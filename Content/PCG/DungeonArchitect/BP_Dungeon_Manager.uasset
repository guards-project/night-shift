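; Dungeon manager that builds the Dungeon Architect level from a replicated random seed, then readies player starts, players and a city backdrop.
; Once loaded, the authority maps the selected crisis to a mission type, spawning its objective actor.
; Mission setup activates shuffled, tag- or class-filtered gameplay markers, with counts scaled by player count.
; Anarchy level changes trigger capped, staggered repop spawns; achievement progressors spawn for patrols and districts.
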(event AnarchyLevelChanged(BP_AnarchyLevel_Component)
  (params (Level :type Integer))
  ;[1 1 1] Repop once only in round (either from BP_RepopTrigger or from last objective event)
  (Spawners|ActivateRepopSpawners))

(event Custom|Set%20Mission%20Type
  (params (Mission%20Type :type E_MissionType%20Enum :default "NewEnumerator0"))
  (Variables|State|SetMission%20Type Mission%20Type)
  (Utilities|FlowControl|Delay 0.2)
  (switch Utilities|FlowControl|Switch|SwitchonE_MissionType (Variables|State|GetMission%20Type)
    (:NewEnumerator0
      (Mission|InitSubduePerps)
      ;[1 1 1] Temp
      ; This activates markers for the desturction mission in other missions to keep the narrative alive!
      (CallFunction|ActivateMarkersOfClass 0 0 "Destroy" :!label _label)
      (Utilities|FlowControl|Delay 1.0)
      (CallFunction|EnableObjectiveItemPhysics))
    (:NewEnumerator3
      (Mission|InitGatherEvidence))
    (:NewEnumerator4
      (Mission|InitDestructionMission)
      (goto _label))
    (:NewEnumerator8
      (Mission|InitHostageRescue)
      (goto _label))
    (:NewEnumerator2
      (Mission|InitWaves)
      (goto _label))
    (:NewEnumerator11
      (Mission|InitArrestTargets)
      (goto _label))))

(event Custom|On%20Crisis%20Selected
  (params (Comp :type BP%20Crisis%20Component%20Object%20Reference))
  (Variables|Default|SetCrisis%20Comp Comp)
  (CallFunction|ApplyDistrictAchievements)
  (if (CallFunction|HasAuthority)
    (Variables|Default|SetArrest%20Row (.ArrestPerp (Utilities|Struct|BreakF_CrisisMission (Default|GetSelectedMission (Variables|Default|GetCrisis%20Comp)))))
    (if (Utilities|Enum|NotEqual(Enum) (select (or (Class|KismetSystemLibrary|IsPackagedforDistribution) (not (Variables|Default|GetUse%20Debug%20Mission))) (.Mission (Utilities|Struct|BreakF_CrisisMission (Default|GetSelectedMission (Variables|Default|GetCrisis%20Comp)))) (Variables|Default|GetDebug%20Mission)) "NewEnumerator10")
      (CallFunction|SetMissionType (select (or (Class|KismetSystemLibrary|IsPackagedforDistribution) (not (Variables|Default|GetUse%20Debug%20Mission))) (.Mission (Utilities|Struct|BreakF_CrisisMission (Default|GetSelectedMission (Variables|Default|GetCrisis%20Comp)))) (Variables|Default|GetDebug%20Mission))))))

(event Custom|Repop
  ;[1 1 1] Repop once only in round (either from BP_RepopTrigger or from last objective event)
)

(event Custom|Dungeon%20Loaded
  (Utilities|FlowControl|Sequence
    (:then_0
      (Networking|SwitchHasAuthority
        (:Authority
          (Utilities|FlowControl|Delay 1.0)
          (Variables|State|SetIs%20Loaded true)
          (Flow|SetGameModeReady))))
    (:then_1
      (Utilities|FlowControl|Delay 1.0)
      (bind _asbp_player_controller_template (Utilities|Casting|CastToBP_PlayerController_Template (Game|GetPlayerController 0)))
      (Default|SetDungeonReady _asbp_player_controller_template true)
      (CallFunction|EnableObjectiveItemPhysics))
    (:then_2
      (CallFunction|BindtoCrisis))))

(event Custom|Bind%20to%20Crisis
  (bind _selected (CallFunction|BindtoCrisisSelected (delegate Custom|On%20Crisis%20Selected)))
  (Utilities|IsValid _selected
    (:Is%20Valid
      (CallFunction|OnCrisisSelected _selected))))

(event EventBeginPlay
  (Utilities|FlowControl|Delay 1.0)
  (Networking|SwitchHasAuthority
    (:Authority
      (Variables|State|SetSeed (Math|Random|RandomInteger 100000))
      (Flow|BindtoAllMissionsComplete)
      (bind _returnvalue (Actor|GetActorOfClass "/Game/UltraDynamicSky/Blueprints/Ultra_Dynamic_Weather.Ultra_Dynamic_Weather_C"))
      (Utilities|IsValid _returnvalue
        (:Is%20Valid
          (EventDispatchers|BindEventtoStartedSnowing _returnvalue (EventDispatchers|CreateEvent :!event CheckforSnowballs))
          (EventDispatchers|BindEventtoFinishedSnowing _returnvalue (EventDispatchers|CreateEvent :!event OnFInishedSnowing)))))))

(fn ConstructionScript)

(fn OnRepSeed
  (bind _returnvalue (Actor|GetActorOfClass "/Script/DungeonArchitectRuntime.Dungeon")) ; looking for SNAP MAP DUNGEON
  (Variables|/Script/DungeonArchitectRuntime.DungeonConfig|SetSeed (Variables|/Script/DungeonArchitectRuntime.Dungeon|GetConfig _returnvalue) (Variables|State|GetSeed))
  (EventDispatchers|BindEventtoOnInitialChunksLoaded (Variables|/Script/DungeonArchitectRuntime.Dungeon|GetLevelStreamingModel _returnvalue) (EventDispatchers|CreateEvent :!event OnDungeonLoaded))
  (Class|Dungeon|BuildDungeon _returnvalue))

(fn SetGameModeReady
  (bind _asbp_game_mode_template_dungeon (Utilities|Casting|CastToBP_GM_NightShift (Game|GetGameMode)))
  (bind _outactors (Actor|GetAllActorsOfClass "/Script/Engine.PlayerStart"))
  (Variables|/Game/_NightShift/BP_GM_NightShift.BP_GM_NightShift_C|SetSpawn%20Room%20Starts _asbp_game_mode_template_dungeon _outactors))

(fn OnRepIsLoaded
  (if (Variables|State|GetIs%20Loaded)
    (Default|CallLoaded)
    (Achievements|FirstOnlinePatrolAchievement)))

(fn BindtoAllMissionsComplete
  (bind _returnvalue (Game|GetGameState))
  (Utilities|IsValid _returnvalue
    (:Is%20Valid
      (bind _asbp_game_state_guards (Utilities|Casting|CastToBP_GameState_Guards _returnvalue))
      (bind _output_get (Variables|Default|SetMission%20Registry (Variables|/Game/Blueprints/Core/BP_GameState_Guards.BP_GameState_Guards_C|GetBP_MissionRegistry_Component_Guards _asbp_game_state_guards)))
      (EventDispatchers|BindEventtoAllMissionsComplete _output_get (EventDispatchers|CreateEvent :!event OnAllMissionsComplete))
      (bind _all_complete (Default|CheckAllMissionsCompete _output_get))
      (if _all_complete
        (Flow|OnAllMissionsComplete (Variables|Default|GetMission%20Registry))))
    (:Is%20Not%20Valid
      (Utilities|Time|SetTimerbyEvent (EventDispatchers|CreateEvent :!event BindtoAllMissionsComplete) 1.0))))

(fn OnAllMissionsComplete
  (params (Registry :type BP%20Mission%20Registry%20Component%20Object%20Reference))
  (CallFunction|Repop))

(fn OnDungeonLoaded
  (params (Dungeon :type Dungeon%20Object%20Reference))
  (CallFunction|DungeonLoaded)
  (Ambient|CreateCityBackdrop))

(fn GetMarkersOfClass
  (params (Class :type Actor%20Class%20Reference))
  (bind _outactors (Actor|GetAllActorsOfClass "/Game/Blueprints/Level/Gameplay/BP_GameplayMarker.BP_GameplayMarker_C"))
  (for _array_element _outactors
    (if (Utilities|Array|ContainsItem (Variables|/Game/Blueprints/Level/Gameplay/BP_GameplayMarker.BP_GameplayMarker_C|GetActor _array_element) Class)
      (Utilities|Array|Add (LocalVariables|GetL%20Markers) _array_element)))
  (return (LocalVariables|GetL%20Markers)))

(fn ActivateEnemySpawners
  (bind _outputpin (CallFunction|GetAllowedEnemyMarkers))
  (LocalVariables|SetL%20Enemy%20Spawners _outputpin)
  (Utilities|FlowControl|Sequence
    (:then_0
      (Utilities|Array|Shuffle (LocalVariables|GetL%20Enemy%20Spawners))
      (Utilities|Array|Resize (LocalVariables|GetL%20Enemy%20Spawners) (Math|Integer|Min(Integer) (Utilities|Array|Length (LocalVariables|GetL%20Enemy%20Spawners)) (.Enemy%20Count (Mission|GetDifficultyCounts)))))
    (:then_1
      (switch Utilities|FlowControl|Switch|SwitchonE_MissionType (Variables|State|GetMission%20Type)
        (:NewEnumerator0
          (Spawners|SubdueReplaceEnemies (LocalVariables|GetL%20Enemy%20Spawners)))
        (:NewEnumerator3
          (Spawners|CollectReplaceEnemies (LocalVariables|GetL%20Enemy%20Spawners)))))
    (:then_2
      (Class|BPIActivation|TriggerActivate(Message) (LocalVariables|GetL%20Enemy%20Spawners) self)
      (return (LocalVariables|GetL%20Enemy%20Spawners)))))

(fn GetDifficultyCounts
  (bind _returnvalue (CallFunction|GetCrisisComponent))
  (bind _crisis_save (Default|GetCrisisSave _returnvalue))
  (LocalVariables|SetL%20Count (Math|Integer|Clamp(Integer) (Variables|/Game/Blueprints/Crisis/BP_SaveGame_Crisis.BP_SaveGame_Crisis_C|GetPlayer%20Count _crisis_save) 1 4))
  (return (* (LocalVariables|GetL%20Count) (Variables|Config|Normal|GetSpawned%20Enemy%20Count)) (+ (* (LocalVariables|GetL%20Count) (Variables|Config|Normal|GetSubdue%20Count)) 10) (+ (* (LocalVariables|GetL%20Count) (Variables|Config|Normal|GetHostage%20Count)) 1) (+ (* (LocalVariables|GetL%20Count) (Variables|Config|Normal|GetEvidence%20Collect%20Count)) 6) (* (LocalVariables|GetL%20Count) (Variables|Config|Normal|GetEvidence%20Collect%20Count)) (+ (+ (* (LocalVariables|GetL%20Count) (Variables|Config|Normal|GetDestruction%20Target%20Count)) 10) 6) (+ (* (LocalVariables|GetL%20Count) (Variables|Config|Normal|GetDestruction%20Target%20Count)) 10) (+ (* (LocalVariables|GetL%20Count) (Variables|Config|Normal|GetArrest%20Count)) 10) (Variables|Config|Normal|GetNormal%20Wave%20Config) (Variables|Config|Normal|GetNormal%20Wave%20Counts)))

(fn InitHostageRescue
  (Spawners|ActivateEnemySpawners)
  (bind _out_markers (Spawners|GetMarkersOfClass "/Game/Blueprints/Core/PolygonAI/BP_Polygon_AI_Civilian.BP_Polygon_AI_Civilian_C"))
  (LocalVariables|SetL%20Escort%20Spawners _out_markers)
  (Utilities|Array|Shuffle (LocalVariables|GetL%20Escort%20Spawners))
  (Utilities|Array|Resize (LocalVariables|GetL%20Escort%20Spawners) (Math|Integer|Min(Integer) (Utilities|Array|Length (LocalVariables|GetL%20Escort%20Spawners)) (.Hostage%20Count (Mission|GetDifficultyCounts))))
  (bind _returnvalue (Game|SpawnActorfromClass "/Game/Blueprints/Gameflow/Objective_Escort/BP_Mission_Escort.BP_Mission_Escort_C" (CallFunction|GetObjectiveSpawnTransform) "AlwaysSpawn" "MultiplyWithRoot" 0 (Variables|MissionData|GetRescue%20Data) -1.0 0))
  (Default|BindtoGameplayMarkers _returnvalue (LocalVariables|GetL%20Escort%20Spawners))
  (Default|TriggerActivate _returnvalue self)
  (Class|BPIActivation|TriggerActivate(Message) (LocalVariables|GetL%20Escort%20Spawners) self))

(fn InitGatherEvidence
  (Spawners|ActivateEnemySpawners)
  (bind _out_markers (Spawners|GetMarkerswithTag "Collect"))
  (LocalVariables|SetL%20Markers _out_markers)
  (Utilities|Array|Shuffle (LocalVariables|GetL%20Markers))
  (Utilities|Array|Resize (LocalVariables|GetL%20Markers) (Math|Integer|Min(Integer) (Utilities|Array|Length (LocalVariables|GetL%20Markers)) (.Evidence%20Spawn%20Count (Mission|GetDifficultyCounts))))
  (bind _returnvalue (Game|SpawnActorfromClass "/Game/Blueprints/Gameflow/Objective_Escort/BP_Mission_Escort.BP_Mission_Escort_C" (CallFunction|GetObjectiveSpawnTransform) "AlwaysSpawn" "MultiplyWithRoot" 0 (Variables|MissionData|GetNarcotics%20Data) -1.0 0))
  (Variables|/Game/Blueprints/Gameflow/Objective_Escort/BP_Mission_Escort.BP_Mission_Escort_C|SetMax%20Targets _returnvalue (Math|Integer|Min(Integer) (Utilities|Array|Length (LocalVariables|GetL%20Markers)) (.Evidence%20Collect%20Count (Mission|GetDifficultyCounts))))
  (Default|BindtoGameplayMarkers _returnvalue (LocalVariables|GetL%20Markers))
  (Default|TriggerActivate _returnvalue self)
  (Class|BPIActivation|TriggerActivate(Message) (LocalVariables|GetL%20Markers) self))

(fn InitSubduePerps
  (Spawners|ActivateEnemySpawners)
  (bind _returnvalue (Game|SpawnActorfromClass "/Game/Blueprints/Gameflow/Objective_ClearRoom/BP_Mission_ClearRoom.BP_Mission_ClearRoom_C" (CallFunction|GetObjectiveSpawnTransform) "AlwaysSpawn" "MultiplyWithRoot" 0 (Variables|MissionData|GetSubdue%20Data) -1.0 0))
  (Variables|/Game/Blueprints/Gameflow/Objective_ClearRoom/BP_Mission_ClearRoom.BP_Mission_ClearRoom_C|SetTarget%20Class _returnvalue (Utilities|Array|MakeArray "/Game/Blueprints/Core/PolygonAI/BP_Polygon_AI.BP_Polygon_AI_C"))
  (bind _outactors (Actor|GetAllActorswithTag "AI"))
  (bind _output_get (Variables|/Game/Blueprints/Gameflow/Objective_ClearRoom/BP_Mission_ClearRoom.BP_Mission_ClearRoom_C|SetTargets _returnvalue _outactors))
  (Variables|/Game/Blueprints/Gameflow/Objective_ClearRoom/BP_Mission_ClearRoom.BP_Mission_ClearRoom_C|SetMax%20Targets _returnvalue (Math|Integer|Min(Integer) (Utilities|Array|Length _output_get) (.Subdue%20Count (Mission|GetDifficultyCounts))))
  (Default|TriggerActivate _returnvalue self))

(fn ReplaceEnemies
  (params (Array :type Array%20of%20BP%20Gameplay%20Marker%20Object%20References) (Chance%20to%20Replace :type Float%20%28double-precision%29) (Find :type Data%20Table%20Row%20Handle%20Structure) (Replace :type F%20Random%20Row%20Config%20Structure))
  (for _array_element Array
    (for (_array_element_2 _array_index) (Variables|/Game/Blueprints/Level/Gameplay/BP_GameplayMarker.BP_GameplayMarker_C|GetRandom%20Data%20Table%20Row _array_element)
      (if (== (.RowName (Utilities|Struct|BreakDataTableRowHandle (.Handle (Utilities|Struct|BreakF_RandomRowConfig _array_element_2)))) (.rowname Find))
        (if (Math|Random|RandomBoolwithWeight Chance%20to%20Replace)
          (Utilities|Array|SetArrayElem (Variables|/Game/Blueprints/Level/Gameplay/BP_GameplayMarker.BP_GameplayMarker_C|GetRandom%20Data%20Table%20Row _array_element) _array_index Replace))))))

(fn SubdueReplaceEnemies
  (params (Array :type Array%20of%20BP%20Gameplay%20Marker%20Object%20References))
  (Spawners|ReplaceEnemies Array 0.5 (LocalVariables|GetL%20Find) (LocalVariables|GetL%20Replace)))

(fn CollectReplaceEnemies
  (params (Array :type Array%20of%20BP%20Gameplay%20Marker%20Object%20References))
  (Spawners|ReplaceEnemies Array 0.5 (LocalVariables|GetL%20Find) (LocalVariables|GetL%20Replace)))

(fn CreateCityBackdrop
  (Networking|CanExecuteCosmeticEvents
    (:True
      (bind _returnvalue (Game|GetCurrentLevelName true))
      (LocalVariables|SetL%20Current%20Level _returnvalue)
      (bind _keys (Utilities|Map|Keys (Variables|Default|GetBackdrop%20|%20Level%20Name)))
      (for _array_element _keys
        (if (Utilities|Enum|Equal(Enum) (.Value (Utilities|Map|Find (Variables|Default|GetBackdrop%20|%20Level%20Name) _array_element)) (LocalVariables|GetL%20Current%20Level))
          (Utilities|Array|Add (LocalVariables|GetL%20Backdrops) _array_element)))
      (Game|SpawnActorfromClass (.OutItem (Utilities|Array|Random (LocalVariables|GetL%20Backdrops))) (Math|Transform|MakeTransform "0, 0, 0" "0, 0, 0" "500.000000,500.000000,20.000000") "AlwaysSpawn" "MultiplyWithRoot" 0 0))))

(fn CheckforSnowballs
  (Networking|SwitchHasAuthority
    (:Authority
      (if (Variables|State|GetIs%20Loaded)
        (bind _returnvalue (Actor|GetActorOfClass "/Game/UltraDynamicSky/Blueprints/Ultra_Dynamic_Weather.Ultra_Dynamic_Weather_C"))
        (Utilities|IsValid _returnvalue
          (:Is%20Valid
            (if (> (Variables|/Game/UltraDynamicSky/Blueprints/Weather_Effects/System/UDS_Weather_Settings.UDS_Weather_Settings_C|GetSnow (Variables|/Game/UltraDynamicSky/Blueprints/Ultra_Dynamic_Weather.Ultra_Dynamic_Weather_C|GetLocal%20Weather%20State _returnvalue)) 0.0)
              (Game|SpawnActorfromClass "/Game/Blueprints/Crisis/PCG/BP_PCG_Snowballs.BP_PCG_Snowballs_C" (CallFunction|GetObjectiveSpawnTransform) "AlwaysSpawn" "MultiplyWithRoot" 0 0))))))))

(fn OnFinishedSnowing
  (bind _outactors (Actor|GetAllActorsOfClass "/Game/Blueprints/Items/Melee/Melee_Sticky/BP_MeleeWeapon_Snowball.BP_MeleeWeapon_Snowball_C"))
  (for _array_element _outactors
    (Default|MCPop _array_element)))

(fn FirstOnlinePatrolAchievement
  (if (not (Class|KismetSystemLibrary|IsStandalone))
    (Game|SpawnActorfromClass "/Game/_Guards/OnlineSubsystem/Achievements/BP_AchievementProgressor.BP_AchievementProgressor_C" (Math|Conversions|ToTransform(Vector) "0, 0, 0") "AlwaysSpawn" "MultiplyWithRoot" 0 "" "FirstPatrol" 0 0)))

(fn ActivateRepopSpawners
  (Networking|SwitchHasAuthority
    (:Authority
      (bind _returnvalue (CallFunction|GetCrisisComponent))
      (Default|GetCrisisSave _returnvalue)
      (LocalVariables|SetL%20Count (Math|Integer|Min(Integer) (Math|Integer|SelectInt 20 10 (>= (Variables|/Game/PCG/DungeonArchitect/BP_AnarchyLevel_Component.BP_AnarchyLevel_Component_C|GetAnarchy%20level (Variables|Default|GetBP_AnarchyLevel_Component)) 5)) (- 80 (CallFunction|GetLivingBots))))
      (bind _outactors (Actor|GetAllActorsOfClasswithTag "/Game/Blueprints/Level/Gameplay/BP_GameplayMarker.BP_GameplayMarker_C" "Repop"))
      (LocalVariables|SetL%20Repop%20Spawners _outactors)
      (Utilities|Array|Shuffle (LocalVariables|GetL%20Repop%20Spawners))
      (Utilities|Array|Resize (LocalVariables|GetL%20Repop%20Spawners) (Math|Integer|Min(Integer) (LocalVariables|GetL%20Count) (Utilities|Array|Length (LocalVariables|GetL%20Repop%20Spawners))))
      (for _array_element (LocalVariables|GetL%20Repop%20Spawners)
        (Default|DelaySpawn _array_element (Math|Random|RandomFloatinRange 0.0 5.0))))))

(fn InitWaves
  (bind (_enemy_count _subdue_count _hostage_count _evidence_spawn_count _evidence_collect_count _destruction_spawn_count _destruction_target_count _arrest_count _wave_configs _wave_counts) (Mission|GetDifficultyCounts))
  (bind _returnvalue (Game|SpawnActorfromClass "/Game/Blueprints/Gameflow/Objective_Waves/BP_Mission_Waves.BP_Mission_Waves_C" (Math|Conversions|ToTransform(Vector) "0, 0, 0") "AlwaysSpawn" "MultiplyWithRoot" 0 _wave_configs _wave_counts (Mission|GetWavesPathNode) (Variables|MissionData|GetWave%20Data) -1.0 0))
  (Default|TriggerActivate _returnvalue self))

(fn GetWavesPathNode
  (bind _outactors (Actor|GetAllActorswithTag "WavesPathNode"))
  (return (.AsBP%20Path%20Node (Utilities|Casting|CastToBP_PathNode (.OutItem (Utilities|Array|Random _outactors))))))

(fn InitDestructionMission
  (Spawners|ActivateEnemySpawners)
  (bind _out_markers (Spawners|GetMarkerswithTag "Destroy"))
  (bind _output_get (LocalVariables|SetL%20Destroy%20Markers _out_markers))
  (Utilities|Array|Shuffle (LocalVariables|GetL%20Destroy%20Markers))
  (Utilities|Array|Resize _output_get (Math|Integer|Min(Integer) (Utilities|Array|Length (LocalVariables|GetL%20Destroy%20Markers)) (.Destruction%20Spawn%20Count (Mission|GetDifficultyCounts))))
  (bind _returnvalue (Game|SpawnActorfromClass "/Game/Blueprints/Gameflow/Objective_ClearRoom/BP_Mission_ClearRoom.BP_Mission_ClearRoom_C" (CallFunction|GetObjectiveSpawnTransform) "AlwaysSpawn" "MultiplyWithRoot" 0 (Variables|MissionData|GetDestroy%20Data) -1.0 0))
  (Variables|/Game/Blueprints/Gameflow/Objective_ClearRoom/BP_Mission_ClearRoom.BP_Mission_ClearRoom_C|SetMax%20Targets _returnvalue (Math|Integer|Min(Integer) (Utilities|Array|Length (LocalVariables|GetL%20Destroy%20Markers)) (.Destruction%20Target%20Count (Mission|GetDifficultyCounts))))
  (Default|BindtoGameplayMarkers _returnvalue (LocalVariables|GetL%20Destroy%20Markers))
  (Class|BPIActivation|TriggerActivate(Message) _returnvalue self)
  (Class|BPIActivation|TriggerActivate(Message) (LocalVariables|GetL%20Destroy%20Markers) self))

(fn InitArrestTargets
  (bind _spawners (Spawners|ActivateEnemySpawners)) ; regular enemies
  (LocalVariables|SetL%20Arrest%20Spawners _spawners)
  ;[1 1 1] Setup the mission
  (bind _returnvalue (Game|SpawnActorfromClass "/Game/Blueprints/Gameflow/Objective_Escort/BP_Mission_Escort.BP_Mission_Escort_C" (Math|Conversions|ToTransform(Vector) "0, 0, 0") "AlwaysSpawn" "MultiplyWithRoot" 0 (Variables|MissionData|GetArrest%20Data) -1.0 0))
  (Variables|/Game/Blueprints/Gameflow/Objective_Escort/BP_Mission_Escort.BP_Mission_Escort_C|SetTarget%20Class _returnvalue (Utilities|Array|MakeArray "/Game/Blueprints/Core/PolygonAI/BP_Polygon_AI.BP_Polygon_AI_C"))
  (Variables|/Game/Blueprints/Gameflow/Objective_Escort/BP_Mission_Escort.BP_Mission_Escort_C|SetMax%20Targets _returnvalue (Math|Integer|Min(Integer) (.Arrest%20Count (Mission|GetDifficultyCounts)) (Utilities|Array|Length (LocalVariables|GetL%20Arrest%20Spawners))))
  (Default|BindtoGameplayMarkers _returnvalue (LocalVariables|GetL%20Arrest%20Spawners))
  (Default|TriggerActivate _returnvalue self))

(fn ActivateMarkersOfClass
  (params (Min :type Integer) (Max :type Integer) (Tag :type Name))
  (bind _outactors (Actor|GetAllActorsOfClasswithTag 0 Tag))
  (LocalVariables|SetL%20Markers _outactors)
  (Utilities|Array|Shuffle (LocalVariables|GetL%20Markers))
  (Utilities|Array|Resize (LocalVariables|GetL%20Markers) (Math|Random|RandomIntegerinRange Min Max))
  (Class|BPIActivation|TriggerActivate(Message) (LocalVariables|GetL%20Markers) self))

(fn GetMarkerswithTag
  (params (Tag :type Name))
  (bind _outactors (Actor|GetAllActorsOfClass "/Game/Blueprints/Level/Gameplay/BP_GameplayMarker.BP_GameplayMarker_C"))
  (for _array_element _outactors
    (if (Actor|ActorHasTag _array_element Tag)
      (Utilities|Array|Add (LocalVariables|GetL%20Markers) _array_element)))
  (return (LocalVariables|GetL%20Markers)))

(fn EnableObjectiveItemPhysics
  ;[1 1 1] next fest 2024 hcks
  (Utilities|FlowControl|Sequence
    (:then_0
      (bind _outactors (Actor|GetAllActorsOfClass "/Game/Blueprints/Fracture/Holdable/BP_Fracture_Crate_Narcotics.BP_Fracture_Crate_Narcotics_C"))
      (Default|ForceUpdatePhysics _outactors))
    (:then_1
      (bind _outactors_2 (Actor|GetAllActorsOfClass "/Game/Blueprints/Fracture/Holdable/BP_Fracture_Crate_FairyCage.BP_Fracture_Crate_FairyCage_C"))
      (Default|ForceUpdatePhysics _outactors_2))
    (:then_2
      (bind _outactors_3 (Actor|GetAllActorsOfClass "/Game/Blueprints/Fracture/Holdable/BP_Fracture_Crate_FairyOre.BP_Fracture_Crate_FairyOre_C"))
      (Default|ForceUpdatePhysics _outactors_3))))

(fn GetAllowedEnemyMarkers
  (bind _out_markers (Spawners|GetMarkersOfClass "/Game/Blueprints/Core/PolygonAI/BP_Polygon_AI.BP_Polygon_AI_C"))
  (for _array_element _out_markers
    (if (and (not (Actor|ActorHasTag _array_element "Repop")) (not (Actor|ActorHasTag _array_element "Terminal")))
      (Utilities|Array|Add (LocalVariables|GetL%20Enemy%20Spawners) _array_element)))
  (return (LocalVariables|GetL%20Enemy%20Spawners)))

(fn ApplyDistrictAchievements
  (Game|SpawnActorfromClass "/Game/_Guards/OnlineSubsystem/Achievements/BP_AchievementProgressor.BP_AchievementProgressor_C" (Math|Conversions|ToTransform(Vector) "0, 0, 0") "AlwaysSpawn" "MultiplyWithRoot" 0 "" (Utilities|String|ToString(Name) (Utilities|Select :Index (Variables|/Game/Blueprints/Crisis/BP_Crisis_Component.BP_Crisis_Component_C|GetDistrict%20ID (Variables|Default|GetCrisis%20Comp)) :Option%200 "First_Patrol_District1" :Option%201 "First_Patrol_District2" :Option%202 "First_Patrol_District3")) 0 0))

(fn GetObjectiveSpawnTransform
  (return (Math|Conversions|ToTransform(Vector) "0.000000,0.000000,5000.000000")))

(fn GetLivingBots
  (bind _outactors (Actor|GetAllActorswithTag "AI"))
  (for _array_element _outactors
    (bind _dead (Class|BPICharacter|IsDead(Message) _array_element))
    (if (not _dead)
      (Math|Integer|IncrementInt (LocalVariables|GetL%20Len)))))