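; Dungeon component that tracks an anarchy level, raising it over time up to a fixed cap.
; On the authority, a looping timer, with an interval set by the enemy-frequency balance cvar (difficulty), drives the increase.
; Each increase also stamps the reinforcement start and end times in server world time.
; The level's OnRep broadcasts a change event to listeners.
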(event `self.ReceiveBeginPlay`
  (`/Engine/EditorBlueprintResources/ActorComponentMacros.Switch Has Authority`
    (:`Authority`
      (bind _returnvalue (`KismetSystemLibrary.K2_SetTimerDelegate` (`|CreateDelegate` :!event `Increase Anarchy Level`) (`KismetMathLibrary.Conv_IntToDouble` (* (select `int` (`ConsoleUtils.GetIntCVar` "Balance.EnemyFreq") :`0` 6 :`1` 4 :`2` 2) 60)) true))
      (set `self.Increase Timer` _returnvalue)
      (`self.Update Start End Time`))))

(fn `Increase Anarchy Level`
  (set `self.Anarchy level` (`KismetMathLibrary.Min` (+ (`self.Anarchy level`) 1) 5))
  (`self.Update Start End Time`))

(fn `OnRep_Anarchy level`
  (`self.Anarchy level Changed` (`self.Anarchy level`)))

(fn `Update Start End Time`
  (set `self.Reinforce Start Time` (`GameStateBase.GetServerWorldTimeSeconds` (`GameplayStatics.GetGameState`)))
  (set `self.Reinforce End Time` (+ (`KismetMathLibrary.Conv_IntToDouble` (* (select `int` (`ConsoleUtils.GetIntCVar` "Balance.EnemyFreq") :`0` 6 :`1` 4 :`2` 2) 60)) (`self.Reinforce Start Time`))))