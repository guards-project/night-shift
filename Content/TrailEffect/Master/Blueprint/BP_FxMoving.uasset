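; BP_FxMoving is an actor that moves a Niagara trail effect along world X, likely to preview trail effects in motion.
; The construction script assigns the chosen Niagara asset and passes its width scale and lifetime as float parameters.
; On BeginPlay it stores the root position and plays the MoveAlpha timeline, lerping the root between plus and minus MoveDistance around that point.
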(event `self.ReceiveBeginPlay`
  (bind _defaultsceneroot (`self.DefaultSceneRoot`))
  (bind _returnvalue (`KismetMathLibrary.MakeVector` (`self.MoveDistance`)))
  (bind _output_get (set `self.RootPosition` (`SceneComponent.K2_GetComponentLocation` _defaultsceneroot)))
  (bind (_direction _alpha) (`Timeline|MoveAlpha`)
    (:`Update`
      (`SceneComponent.K2_SetWorldLocation` _defaultsceneroot (`KismetMathLibrary.VLerp` (+ _output_get _returnvalue) (- _output_get _returnvalue) _alpha) false false))))

(fn `UserConstructionScript`
  (bind _niagara (`self.Niagara`))
  (`NiagaraComponent.SetAsset` _niagara (`self.NiagaraFx_Trail`) true)
  (`NiagaraComponent.SetVariableFloat` _niagara "EffectWidthScale" (`self.EffectWidthScale`))
  (`NiagaraComponent.SetVariableFloat` _niagara "LifeTime" (`self.LifeTime`)))