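; Mission registry component that keeps a replicated list of missions and signals when all of them are complete.
; Registering or unregistering binds or unbinds each mission's state-change event and broadcasts a registry change, also fired on replication.
; State changes trigger a completion check that requires at least one eligible mission, with eligibility currently always true.
; It can also destroy every mission actor, while its mission-list UI creation is unused, deferring to the player HUD.
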(event `self.ReceiveBeginPlay`)

(fn `Can Trigger All Missions Complete`
  (params (Mission :type "/Game/Primer/Primer_MissionHierarchy/BP_Mission Object Reference"))
  (returns (OutputPin :type Boolean))
  (return true))

(fn `Check All Missions Compete`
  (returns (`All Complete` :type Boolean))
  (locals (`L Found A Mission` :type Boolean :default false))
  ;[1 1 1] Check All Mission Complete
  (for _array_element (`self.Registered Missions`)
    (if (`self.Can Trigger All Missions Complete` _array_element)
      (set `local.L Found A Mission` true)
      (if (not (`/Game/Primer/Primer_MissionHierarchy/BP_Mission.Is Complete` _array_element))
        (return false) ; there is an active mission
      )))
  (return (`local.L Found A Mission`)) ; there is no active mission
)

(fn `Create Mission List UI`
  (`/Engine/EditorBlueprintResources/StandardMacros.Can Execute Cosmetic Events`
    (:`True`
      (bind _returnvalue (`|CreateWidget` "/Game/Primer/Primer_MissionHierarchy/W_Mission_List.W_Mission_List_C" (`GameplayStatics.GetPlayerController` 0)))
      (`UserWidget.SetPositionInViewport` _returnvalue (70.0 0.0) true)
      (`UserWidget.SetAnchorsInViewport` _returnvalue (make `Anchors` (0.0 0.2) (0.0 0.2)))
      (`UserWidget.AddToViewport` _returnvalue -1))))

(fn `Destroy All Missions`
  (for _array_element (`self.Registered Missions`)
    (`/Engine/EditorBlueprintResources/StandardMacros.IsValid` _array_element
      (:`Is Valid`
        (`Actor.K2_DestroyActor` _array_element))))
  (bind _outactors (`GameplayStatics.GetAllActorsOfClass` "/Game/Primer/Primer_MissionHierarchy/BP_Mission.BP_Mission_C"))
  (for _array_element_2 _outactors
    (`/Engine/EditorBlueprintResources/StandardMacros.IsValid` _array_element_2
      (:`Is Valid`
        (`Actor.K2_DestroyActor` _array_element_2)))))

(fn `On Registered Mission State Changed`
  (params (Mission :type "/Game/Primer/Primer_MissionHierarchy/BP_Mission Object Reference") (State :type "/Game/Primer/Primer_MissionHierarchy/E_MissionState Enum" :default "NewEnumerator6"))
  (bind _all_complete (`self.Check All Missions Compete`))
  (if _all_complete
    (`self.All Missions Complete` self)))

(fn `OnRep_Registered Missions`
  (`self.Mission Registry Changed` self))

(fn `Register Mission`
  (params (Mission :type "/Game/Primer/Primer_MissionHierarchy/BP_Mission Object Reference"))
  (`KismetArrayLibrary.Array_AddUnique` (`self.Registered Missions`) Mission)
  (`self.Mission Registry Changed` self)
  (add `/Game/Primer/Primer_MissionHierarchy/BP_Mission.Mission State Changed` Mission (`|CreateDelegate` :!event `On Registered Mission State Changed`)))

(fn `Unregister Mission`
  (params (Mission :type "/Game/Primer/Primer_MissionHierarchy/BP_Mission Object Reference"))
  (bind _returnvalue (`KismetArrayLibrary.Array_RemoveItem` (`self.Registered Missions`) Mission))
  (if _returnvalue
    (`self.Mission Registry Changed` self)
    (remove `/Game/Primer/Primer_MissionHierarchy/BP_Mission.Mission State Changed` Mission (`|CreateDelegate` :!event `On Registered Mission State Changed`))
    (else
      (`KismetSystemLibrary.PrintString` (`KismetStringLibrary.Concat_StrStr` "Error: Cannot Unregister Mission " (`KismetSystemLibrary.GetDisplayName` Mission) " because it is not registered")))))