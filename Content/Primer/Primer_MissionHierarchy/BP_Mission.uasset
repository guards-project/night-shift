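; Base mission actor that loads settings from a data table and registers with the mission registry component on GameState.
; Server-authoritative state drives timed auto-activation, countdown and duration, with duration expiry choosing the outcome.
; Completion fires once, triggers sequenced missions and optionally destroys the actor after a delay.
; RepNotifies broadcast state, server-time timestamp and count changes, letting time remaining derive from replicated timestamps.
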(event `self.ReceiveBeginPlay`
  ;[1 1 1] Start Activate Delay
  (`self.Load Data`)
  (`self.Register Mission`)
  (`self.Init Auto Activate`))

(event `/Game/Primer/Primer_Shared/BPI_Activation.Trigger Activate`
  (params (Context :type "Object Object Reference"))
  ;[1 1 1] Start Activate Delay
  (`self.Start Mission`))

(event `self.ReceiveEndPlay`
  (params (EndPlayReason :type "EEndPlayReason Enum" :default "Destroyed"))
  ;[1 1 1] Start Activate Delay
  (`self.Unregister Mission`))

(event `/Game/Primer/Primer_Shared/BPI_Activation.Trigger Deactivate`
  (params (Context :type "Object Object Reference"))
  ;[1 1 1] Start Activate Delay
  (`self.Stop Mission`))

(event `Init Auto Activate`
  ;[1 1 1] Self Activation and countdown
  (`/Engine/EditorBlueprintResources/ActorMacros.Switch Has Authority`
    (:`Authority`
      (if (>= (`self.Auto Activate Delay`) 0.0)
        (if (> (`self.Auto Activate Delay`) 0.0)
          (bind _returnvalue (`KismetSystemLibrary.K2_SetTimerDelegate` (`|CreateDelegate` :!event `Start Countdown`) (`self.Auto Activate Delay`)))
          (set `self.Mission Timer` _returnvalue)
          (else
            (`self.Start Countdown`)))))))

(event `Start Countdown`
  (bind ((`Countdown_14_416149714AF26DB237848A8C95EBBBD5` _countdown)) (break `/Game/Primer/Primer_MissionHierarchy/F_MissionData` (`self.Mission Data`)))
  ;[1 1 1] Self Activation and countdown
  (`self.Set Mission State` "NewEnumerator8")
  (if (> _countdown 0.0)
    (bind _returnvalue (`KismetSystemLibrary.K2_SetTimerDelegate` (`|CreateDelegate` :!event `Start Mission`) _countdown))
    (set `self.Mission Timer` _returnvalue)
    (set `self.Start Timestamp` (+ (`GameStateBase.GetServerWorldTimeSeconds` (`GameplayStatics.GetGameState`)) (`.Countdown_14_416149714AF26DB237848A8C95EBBBD5` (break `/Game/Primer/Primer_MissionHierarchy/F_MissionData` (`self.Mission Data`)))))
    (else
      (`self.Start Mission`))))

(event `Start Mission`
  (bind _returnvalue (`GameplayStatics.GetGameState`))
  ;[1 1 1] Mission Start and End
  (`/Engine/EditorBlueprintResources/StandardMacros.IsValid` _returnvalue
    (:`Is Valid`
      (set `self.Start Timestamp` (`GameStateBase.GetServerWorldTimeSeconds` _returnvalue))
      (`self.Set Mission State` "NewEnumerator3")
      (`self.Initialize Duration`))))

(event `On Mission State Changed`
  (params (`Mission State` :type "/Game/Primer/Primer_MissionHierarchy/E_MissionState Enum" :default "NewEnumerator6"))
  ;[1 1 1] Mission Start and End
)

(event `Stop Mission`
  ;[1 1 1] Mission Start and End
  (`self.Set Mission State` "NewEnumerator6"))

(event `Complete Mission`
  (params (`Mission State` :type "/Game/Primer/Primer_MissionHierarchy/E_MissionState Enum" :default "NewEnumerator1"))
  ;[1 1 1] Mission Start and End
  (`/Engine/EditorBlueprintResources/StandardMacros.DoOnce` false
    (:`Completed`
      (set `self.Complete Timestamp` (`GameStateBase.GetServerWorldTimeSeconds` (`GameplayStatics.GetGameState`)))
      (`self.Set Mission State` `Mission State`)
      (`self.Post Complete Destroy`)
      (`self.Activate Next Missions`))))

(event `Reset Mission`
  ;[1 1 1] Mission Start and End
  (`self.Start Countdown`))

(event `Activate Next Missions`
  ;[1 1 1] Mission Start and End
  (`/Game/Primer/Primer_Shared/BPI_Activation.Trigger Activate` (`self.Sequenced Missions`) self))

(event `Initialize Duration`
  (bind _out (`self.Get Duration`))
  ;[1 1 1] Duration
  (if (> _out 0.0)
    (bind _returnvalue (`KismetSystemLibrary.K2_SetTimerDelegate` (delegate `Duration Complete`) _out))
    (set `self.Mission Timer` _returnvalue)))

(event `Duration Complete`
  ;[1 1 1] Duration
  (if (`.WinonDurationEnd_12_B31853B646F5BEDEC2A41BB6CCA947BF` (break `/Game/Primer/Primer_MissionHierarchy/F_MissionData` (`self.Mission Data`)))
    (`self.Complete Mission` "NewEnumerator1")
    (else
      (`self.Complete Mission` "NewEnumerator2"))))

(event `Post Complete Destroy`
  (bind ((`PostCompleteDestroyDelay_21_F3DCB7AE48BC7AF6A5D30DAABB42FD61` _postcompletedestroydelay)) (break `/Game/Primer/Primer_MissionHierarchy/F_MissionData` (`self.Mission Data`)))
  ;[1 1 1] Destroy actor after completion
  (if (> _postcompletedestroydelay 0.0)
    (`KismetSystemLibrary.Delay` _postcompletedestroydelay)
    (`self.K2_DestroyActor`)))

(event `Draw Mission Intro`)

(fn `Get Complete Timestamp`
  (returns (`Start Timestamp` :type "Float (double-precision)"))
  (return (`self.Complete Timestamp`)))

(fn `Get Duration`
  (returns (Out :type "Float (double-precision)"))
  (bind _duration (`self.Duration`))
  (return (`KismetMathLibrary.SelectFloat` _duration (`.Duration_13_311147654FA5053C54B1D5B0C586B650` (break `/Game/Primer/Primer_MissionHierarchy/F_MissionData` (`self.Mission Data`))) (> _duration 0.0))))

(fn `Get Mission Data`
  (returns (`Mission Data` :type "/Game/Primer/Primer_MissionHierarchy/F_MissionData Structure"))
  (return (`self.Mission Data`)))

(fn `Get Mission State`
  (returns (`Mission State` :type "/Game/Primer/Primer_MissionHierarchy/E_MissionState Enum"))
  (return (`self.Mission State`)))

(fn `Get Start Timestamp`
  (returns (`Start Timestamp` :type "Float (double-precision)"))
  (return (`self.Start Timestamp`)))

(fn `Get Time Remaining`
  (returns (`Mission Duration` :type "Float (double-precision)") (`Time Remaining` :type "Float (double-precision)"))
  (bind _returnvalue (- (`GameStateBase.GetServerWorldTimeSeconds` (`GameplayStatics.GetGameState`)) (`self.Get Start Timestamp`)))
  (return (`self.Get Duration`) (`KismetMathLibrary.FMax` (`KismetMathLibrary.SelectFloat` (- (`self.Get Duration`) (- (`self.Get Complete Timestamp`) (`self.Get Start Timestamp`))) (`KismetMathLibrary.SelectFloat` (`KismetMathLibrary.Abs` _returnvalue) (- (`self.Get Duration`) _returnvalue) (< _returnvalue 0.0)) (`self.Is Complete`)))))

(fn `Is Active`
  (returns (ReturnValue :type Boolean))
  (return (`|EnumEquality` (`self.Mission State`) "NewEnumerator3")))

(fn `Is Complete`
  (returns (ReturnValue :type Boolean))
  (return (> (`KismetMathLibrary.Conv_ByteToInt` (`self.Mission State`)) (`KismetMathLibrary.Conv_ByteToInt` (enumliteral `/Game/Primer/Primer_MissionHierarchy/E_MissionState` "NewEnumerator3")))))

(fn `Is Inactive`
  (returns (ReturnValue :type Boolean))
  (return (`|EnumEquality` (`self.Mission State`) "NewEnumerator6")))

(fn `Load Data`
  (bind (_mission_data_handle_datatable _mission_data_handle_rowname) (break `DataTableRowHandle` (`self.Mission Data Handle`)))
  (bind _returnvalue (`|GetDataTableRow` _mission_data_handle_datatable _mission_data_handle_rowname)
    (:`then`
      (set `self.Mission Data` _returnvalue))
    (:`RowNotFound`
      (`KismetSystemLibrary.PrintString` (`KismetStringLibrary.Concat_StrStr` "Error: Cannot find mission data row: " (`KismetStringLibrary.Conv_NameToString` _mission_data_handle_rowname))))))

(fn `OnRep_Complete Timestamp`
  (`self.Complete Timestamp Changed` self (`self.Complete Timestamp`)))

(fn `OnRep_Current Count`
  (`self.Count Changed` (`self.Current Count`) (`self.Target Count`)))

(fn `OnRep_Mission State`
  (bind _mission_state (`self.Mission State`))
  (`self.On Mission State Changed` _mission_state)
  (`self.Mission State Changed` self _mission_state))

(fn `OnRep_Start Timestamp`
  (`self.Start Timestamp Changed` self (`self.Start Timestamp`)))

(fn `OnRep_Target Count`
  (`self.Count Changed` (`self.Current Count`) (`self.Target Count`)))

(fn `Register Mission`
  (bind _returnvalue (`GameplayStatics.GetGameState`))
  (bind _returnvalue_2 (`self.GetComponentByClass` _returnvalue "/Game/Primer/Primer_MissionHierarchy/BP_MissionRegistry_Component.BP_MissionRegistry_Component_C"))
  (`/Engine/EditorBlueprintResources/StandardMacros.IsValid` _returnvalue
    (:`Is Valid`
      (`/Engine/EditorBlueprintResources/StandardMacros.IsValid` _returnvalue_2
        (:`Is Valid`
          (`/Game/Primer/Primer_MissionHierarchy/BP_MissionRegistry_Component.Register Mission` _returnvalue_2 self)
          (set `self.Mission Registry` _returnvalue_2))))))

(fn `Set Mission State`
  (params (`Mission State` :type "/Game/Primer/Primer_MissionHierarchy/E_MissionState Enum" :default "NewEnumerator6"))
  (`/Engine/EditorBlueprintResources/ActorMacros.Switch Has Authority`
    (:`Authority`
      (if (`|EnumInequality` `Mission State` (`self.Mission State`))
        (`self.State Change Cleanup`)
        (set `self.Mission State` `Mission State`)))))

(fn `Set Title`
  (params (Name :type Text))
  (setmembers `/Game/Primer/Primer_MissionHierarchy/F_MissionData` :`StructRef` (`self.Mission Data`) :`Name` Name))

(fn `State Change Cleanup`
  (`KismetSystemLibrary.K2_ClearAndInvalidateTimerHandle` (`self.Mission Timer`)))

(fn `Unregister Mission`
  (bind _returnvalue (`GameplayStatics.GetGameState`))
  (bind _returnvalue_2 (`self.GetComponentByClass` _returnvalue "/Game/Primer/Primer_MissionHierarchy/BP_MissionRegistry_Component.BP_MissionRegistry_Component_C"))
  (`/Engine/EditorBlueprintResources/StandardMacros.IsValid` _returnvalue
    (:`Is Valid`
      (`/Engine/EditorBlueprintResources/StandardMacros.IsValid` _returnvalue_2
        (:`Is Valid`
          (`/Game/Primer/Primer_MissionHierarchy/BP_MissionRegistry_Component.Unregister Mission` _returnvalue_2 self))))))

(fn `UserConstructionScript`)