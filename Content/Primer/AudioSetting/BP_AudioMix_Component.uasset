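; Audio settings component that applies per-sound-class volume levels to a base Sound Mix on BeginPlay.
; It seeds any sound class missing from the settings save object with its default volume, then applies each stored value as a class override with a short fade.
; The save object is lazily loaded and cached, with the slot deleted and a fresh object created if it is missing or invalid.
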(event `self.ReceiveBeginPlay`
  (`self.Init Sound Mix`))

(fn `Get Audio Save`
  (returns (`AsBP Save Game Audio Settings` :type "/Game/Primer/AudioSetting/BP_SaveGame_AudioSettings Object Reference"))
  (bind _audio_save (`self.Audio Save`)
    (:`then`
      (return _audio_save))
    (:`else`
      (bind _returnvalue (`GameplayStatics.DoesSaveGameExist` (`self.Audio Save Slot Name`)))
      (if _returnvalue
        (bind _returnvalue_2 (`GameplayStatics.LoadGameFromSlot` (`self.Audio Save Slot Name`)))
        (`/Engine/EditorBlueprintResources/StandardMacros.IsValid` _returnvalue_2
          (:`Is Valid`
            (bind _asbp_save_game_audio_settings (cast `/Game/Primer/AudioSetting/BP_SaveGame_AudioSettings` _returnvalue_2)
              (:`then`
                (bind _output_get (set `self.Audio Save` _asbp_save_game_audio_settings))
                (return _output_get))
              (:`CastFailed`
                _)))
          (:`Is Not Valid`
            _)))
      (`GameplayStatics.DeleteGameInSlot` (`self.Audio Save Slot Name`)) ; Safety Delete encase it was corrupt
      (bind _returnvalue_3 (`GameplayStatics.CreateSaveGameObject` "/Game/Primer/AudioSetting/BP_SaveGame_AudioSettings.BP_SaveGame_AudioSettings_C"))
      (bind _output_get_2 (set `self.Audio Save` _returnvalue_3))
      (return _output_get_2))))

(fn `Init Sound Mix`
  (bind _asbp_save_game_audio_settings (`self.Get Audio Save`))
  (bind _audio_class___default_volume (`self.Audio Class | Default Volume`))
  (`GameplayStatics.SetBaseSoundMix` "/Game/Primer/AudioSetting/SoundMix.SoundMix")
  (bind _keys (`BlueprintMapLibrary.Map_Keys` _audio_class___default_volume))
  (for _array_element _keys
    (bind (_value _returnvalue) (`/Game/Primer/AudioSetting/BP_SaveGame_AudioSettings.Get Volume` _asbp_save_game_audio_settings _array_element))
    (if (not _returnvalue)
      (`/Game/Primer/AudioSetting/BP_SaveGame_AudioSettings.Set Volume` _asbp_save_game_audio_settings _array_element (`BlueprintMapLibrary.Map_Find` _audio_class___default_volume _array_element)))
    (`GameplayStatics.SetSoundMixClassOverride` "/Game/Primer/AudioSetting/SoundMix.SoundMix" _array_element _value 1.0 0.2)))