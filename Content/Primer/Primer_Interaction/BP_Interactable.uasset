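; BP_Interactable is an actor that players can focus and interact with, apparently a base for specific interactables.
; Focus events toggle custom depth highlighting on meshes from GetHighlightMeshes, which is empty here.
; Interact start, execute and stop print local-or-server debug text, and execute also fires the Interacted dispatcher.
; Getters expose distance, duration, text and widget settings, while CanInteract's RepNotify calls an event and dispatcher.
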(event `/Game/Primer/Primer_Interaction/BPI_Interact.Start Interact`
  (params (User :type "Controller Object Reference"))
  ;[1 1 1] Interaction
  (`KismetSystemLibrary.PrintString` (`KismetMathLibrary.SelectString` "Local Actor Interact Started" "Server Actor Interact Started" (`Controller.IsLocalPlayerController` User))))

(event `/Game/Primer/Primer_Interaction/BPI_Interact.Execute Interact`
  (params (User :type "Controller Object Reference"))
  ;[1 1 1] Interaction
  (`self.Interacted` self)
  (`KismetSystemLibrary.PrintString` (`KismetMathLibrary.SelectString` "Local Actor Interact Executed" "Server Actor Interact Executed" (`Controller.IsLocalPlayerController` User)) true true (struct :`R` 1.0 :`G` 0.400337 :`A` 1.0)))

(event `/Game/Primer/Primer_Interaction/BPI_Interact.Stop Interact`
  (params (User :type "Controller Object Reference"))
  ;[1 1 1] Interaction
  (`KismetSystemLibrary.PrintString` (`KismetMathLibrary.SelectString` "Local Actor Interact Stopped" "Server Actor Interact Stopped" (`Controller.IsLocalPlayerController` User))))

(event `/Game/Primer/Primer_Interaction/BPI_Interact.Start Focus`
  ;[1 1 1] Focus
  (`KismetSystemLibrary.PrintString` "Actor Start Focus")
  (`self.Set Mesh Highlight` true))

(event `/Game/Primer/Primer_Interaction/BPI_Interact.Stop Focus`
  ;[1 1 1] Focus
  (`KismetSystemLibrary.PrintString` "Actor Stop Focus")
  (`self.Set Mesh Highlight` false))

(event `On Can Interact Changed`
  (params (CanInteract :type Boolean)))

(fn `Get Always Show Widget`
  (returns (`Always Show` :type Boolean))
  (return (`self.Always Show Interact Widget`)))

(fn `Get Can Interact`
  (returns (ReturnValue :type Boolean))
  (return (`self.Can Interact`)))

(fn `Get Highlight Meshes`
  (returns (Array :type "Array of PrimitiveComponent Object Reference"))
  (return))

(fn `Get Interact Distance`
  (returns (Distance :type "Float (double-precision)"))
  (return (`self.Interact Distance`)))

(fn `Get Interact Duration`
  (returns (Duration :type "Float (double-precision)"))
  (return (`self.Interact Duration`)))

(fn `Get Interact Text`
  (returns (Text :type Text))
  (return (`self.Interact Text`)))

(fn `Get Interact Widget Class`
  (returns (`Widget Class` :type "/Game/Primer/Primer_Interaction/UI/W_Interact_Master Soft Class Reference"))
  (return (`self.Interact Widget Class`)))

(fn `OnRep_Can Interact`
  (bind _can_interact (`self.Can Interact`))
  (`self.On Can Interact Changed` _can_interact)
  (`self.Can Interact Changed` _can_interact))

(fn `Set Mesh Highlight`
  (params (Show :type Boolean))
  (bind _array (`self.Get Highlight Meshes`))
  (if (`KismetArrayLibrary.Array_IsValidIndex` _array)
    (`PrimitiveComponent.SetRenderCustomDepth` _array (`local.Show`))))

(fn `UserConstructionScript`)