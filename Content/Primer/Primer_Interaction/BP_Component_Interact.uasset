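; Pawn interaction component that finds, focuses and triggers actors implementing BPI_Interact.
; While active, it box-traces ahead of the camera each tick, filters hits by availability and distance, and picks the lowest dot against its right vector.
; Focus changes send start/stop messages and cancel ongoing interaction.
; SetInteracting executes immediately or after the target's hold duration via timer, and clients also forward execution through ServerInteract.
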(event `self.ReceiveBeginPlay`
  (bind _aspawn (cast `Pawn` (`self.GetOwner`)))
  (bind _output_get (set `self.Pawn Owner` _aspawn))
  (if (or (`Pawn.IsLocallyControlled` _output_get) (`KismetSystemLibrary.IsServer`))
    (`self.SetComponentTickEnabled` true)
    (add `self.OnComponentDeactivated` (delegate `On Deactivate`))
    (add `self.OnComponentActivated` (delegate `On Activate`))))

(event `On Deactivate` :!signature `self.OnComponentDeactivated`
  (params (Component :type "ActorComponent Object Reference"))
  (`self.Set Interacting` false)
  (`self.Clear Traced Actor`))

(event `On Activate` :!signature `self.OnComponentActivated`
  (params (Component :type "ActorComponent Object Reference") (bReset :type Boolean)))

(event `self.ReceiveTick`
  (params (DeltaSeconds :type "Float (single-precision)"))
  (`self.Interact Hit Test`))

(event `Set Interacting`
  (params (Interact :type Boolean))
  (if Interact
    (if (not (`self.Is Interacting`))
      (bind _traced_actor (`self.Traced Actor`)
        (:`then`
          (message `/Game/Primer/Primer_Interaction/BPI_Interact.Start Interact` _traced_actor (`Pawn.GetController` (`self.Pawn Owner`)))
          (set `self.Is Interacting` true)
          (bind _duration (message `/Game/Primer/Primer_Interaction/BPI_Interact.Get Interact Duration` (`self.Traced Actor`)))
          (if (> _duration 0.0)
            (bind _returnvalue (`KismetSystemLibrary.K2_SetTimerDelegate` (`|CreateDelegate` :!event `Interact Duration Complete`) _duration))
            (set `self.Interact Duration Handle` _returnvalue)
            (else
              (`self.Interact Duration Complete`))))
        (:`else`)))
    (elif (`self.Is Interacting`)
      (set `self.Is Interacting` false)
      (bind _traced_actor_2 (`self.Traced Actor`)
        (:`then`
          (message `/Game/Primer/Primer_Interaction/BPI_Interact.Stop Interact` _traced_actor_2 (`Pawn.GetController` (`self.Pawn Owner`)))
          (`KismetSystemLibrary.K2_ClearAndInvalidateTimerHandle` (`self.Interact Duration Handle`)))
        (:`else`)))))

(event `Interact Duration Complete`
  (bind _traced_actor (`self.Traced Actor`)
    (:`then`
      (message `/Game/Primer/Primer_Interaction/BPI_Interact.Execute Interact` _traced_actor (`Pawn.GetController` (`self.Pawn Owner`)))
      (if (not (`KismetSystemLibrary.IsServer`))
        (`self.Server Interact` _traced_actor)))
    (:`else`)))

(event `Server Interact`
  (params (Actor :type "Actor Object Reference"))
  (bind _output_get (set `self.Traced Actor` Actor))
  (message `/Game/Primer/Primer_Interaction/BPI_Interact.Execute Interact` _output_get (`Pawn.GetController` (`self.Pawn Owner`))))

(fn `Can Trace`
  (returns (ReturnValue :type Boolean))
  (bind _pawn_owner (`self.Pawn Owner`)
    (:`then`
      _)
    (:`else`
      _))
  (return (`self.IsActive`)))

(fn `Clear Traced Actor`
  (`self.Traced Actor`
    (:`then`
      (`|ExecutionSequence`
        (:`then_0`
          (message `/Game/Primer/Primer_Interaction/BPI_Interact.Stop Focus` (`self.Traced Actor`))
          (`self.Set Interacting` false))
        (:`then_1`
          (set `self.Traced Actor` null)
          (`self.Focus Changed` null))))
    (:`else`
      (`|ExecutionSequence`
        (:`then_0`
          (if (`self.Is Focussing`)
            (set `self.Is Focussing` false)
            (`self.Focus Changed` null)))
        (:`then_1`
          (if (`self.Is Interacting`)
            (`self.Set Interacting` false)))))))

(fn `Debug Interact Line`
  (params (LineEnd :type "Vector Structure"))
  (if (`|EnumInequality` (`self.Debug Type`))
    (`KismetSystemLibrary.DrawDebugLine` (`Actor.K2_GetActorLocation` (`self.GetOwner`)) LineEnd (struct :`G` 0.13723 :`B` 1.0 :`A` 1.0) 1.0 1.0)))

(fn `Get Dot to Target`
  (params (To :type "Vector Structure"))
  (returns (ReturnValue :type "Float (double-precision)"))
  (if (`self.Dot Ignore Pitch`)
    (return (`KismetMathLibrary.Dot_VectorVector` (`KismetMathLibrary.Vector_Normal2D` (`self.GetRightVector`)) (`KismetMathLibrary.Vector_Normal2D` (`KismetMathLibrary.GetDirectionUnitVector` (`self.K2_GetComponentLocation`) (`local.To`)))))
    (else
      (return (`KismetMathLibrary.Dot_VectorVector` (`self.GetRightVector`) (`KismetMathLibrary.GetDirectionUnitVector` (`self.K2_GetComponentLocation`) (`local.To`)))))))

(fn `Get Trace Actor`
  (returns (`Closest Hit` :type "HitResult Structure"))
  (locals (`L Closest Dot` :type "Float (double-precision)" :default 1.0) (`L Closest Actor` :type "Actor Object Reference") (`L Closest Hit` :type "HitResult Structure"))
  (bind (_start _forward) (`self.Get Trace Direction`))
  (bind _trace_size (`self.Trace Size`))
  (bind _outhits (`KismetSystemLibrary.BoxTraceMulti` _start _start (`KismetMathLibrary.MakeVector` (/ (`self.Trace Distance`) 2.0) _trace_size _trace_size) (`KismetMathLibrary.Conv_VectorToRotator` _forward) "TraceTypeQuery3" true (`self.Get Trace Ignore Actors`) (`self.Debug Type`)))
  (for _array_element _outhits
    (bind (_bblockinghit _binitialoverlap _time _distance _location _impactpoint _normal _impactnormal _physmat _hitactor _hitcomponent) (`GameplayStatics.BreakHitResult` _array_element))
    (if (`KismetSystemLibrary.DoesImplementInterface` _hitactor "/Game/Primer/Primer_Interaction/BPI_Interact.BPI_Interact_C")
      (bind _origin (`KismetSystemLibrary.GetComponentBounds` _hitcomponent))
      (`self.Debug Interact Line` _origin)
      (bind _returnvalue (message `/Game/Primer/Primer_Interaction/BPI_Interact.Get Can Interact` _hitactor))
      (bind _always_show (message `/Game/Primer/Primer_Interaction/BPI_Interact.Get Always Show Widget` _hitactor))
      (if (or _returnvalue _always_show)
        (bind _distance_2 (message `/Game/Primer/Primer_Interaction/BPI_Interact.Get Interact Distance` _hitactor))
        (if (or (== _distance_2 0.0) (<= (`KismetMathLibrary.Vector_Distance` _origin (`Actor.K2_GetActorLocation` (`self.GetOwner`))) _distance_2))
          (bind _returnvalue_2 (`self.Get Dot to Target` _origin))
          (if (< _returnvalue_2 (`local.L Closest Dot`))
            (set `local.L Closest Dot` _returnvalue_2)
            (set `local.L Closest Hit` _array_element))))))
  (return (`local.L Closest Hit`)))

(fn `Get Trace Direction`
  (returns (Start :type "Vector Structure") (Forward :type "Vector Structure"))
  (bind _returnvalue (`GameplayStatics.GetPlayerCameraManager` 0))
  (bind _returnvalue_2 (`KismetMathLibrary.Conv_RotatorToVector` (`PlayerCameraManager.GetCameraRotation` _returnvalue)))
  (return (+ (`PlayerCameraManager.GetCameraLocation` _returnvalue) (* _returnvalue_2 (/ (`self.Trace Distance`) 2.0))) _returnvalue_2))

(fn `Get Trace Ignore Actors`
  (returns (Array :type "Array of Actor Object Reference (by ref)"))
  (return (`|MakeArray` (`self.GetOwner`))))

(fn `Interact Hit Test`
  (if (`self.Can Trace`)
    (bind _closest_hit (`self.Get Trace Actor`))
    (bind (_bblockinghit _binitialoverlap _time _distance _location _impactpoint _normal _impactnormal _physmat _hitactor) (`GameplayStatics.BreakHitResult` _closest_hit))
    (`/Engine/EditorBlueprintResources/StandardMacros.IsValid` _hitactor
      (:`Is Valid`
        (`self.Set Traced Actor` _hitactor))
      (:`Is Not Valid`
        (`self.Clear Traced Actor` :!label _label)))
    (else
      (goto _label))))

(fn `Set Traced Actor`
  (params (`In Traced Actor` :type "Actor Object Reference"))
  (if (!= `In Traced Actor` (`self.Traced Actor`))
    (`self.Clear Traced Actor`)
    (bind _in_traced_actor (`local.In Traced Actor`)
      (:`then`
        (bind _output_get (set `self.Traced Actor` _in_traced_actor))
        (message `/Game/Primer/Primer_Interaction/BPI_Interact.Start Focus` _output_get)
        (`self.Focus Changed` (`self.Traced Actor`))
        (set `self.Is Focussing` true))
      (:`else`))))