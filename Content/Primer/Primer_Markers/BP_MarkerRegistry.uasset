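; BP_MarkerRegistry keeps a central list of markers and announces changes to it through event dispatchers.
; RegisterMarker adds a marker uniquely and fires MarkerRegistered only when it was not already listed.
; UnregisterMarker removes a marker and fires MarkerUnregistered only when a removal happened.
; Both dispatchers pass the registry and the affected marker, and the event graph holds no active logic.
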(fn `Register Marker`
  (params (`New Marker` :type "/Game/Primer/Primer_Markers/BP_Marker Object Reference (by ref)"))
  (bind _returnvalue (`KismetArrayLibrary.Array_AddUnique` (`self.Markers`) `New Marker`))
  (if (!= _returnvalue -1)
    (`self.Marker Registered` self (`local.New Marker`))))

(fn `Unregister Marker`
  (params (Marker :type "/Game/Primer/Primer_Markers/BP_Marker Object Reference (by ref)"))
  (bind _returnvalue (`KismetArrayLibrary.Array_RemoveItem` (`self.Markers`) Marker))
  (if _returnvalue
    (`self.Marker Unregistered` self (`local.Marker`))))