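; BP_Marker is a marker that adds or removes itself from the BP_MarkerRegistry component on the local player's HUD.
; On BeginPlay and whenever the replicated IsRegistered flag triggers its OnRep, it registers or unregisters to match the flag; EndPlay always unregisters.
; Both operations reach the registry through player controller 0, acting only if that controller is local and the HUD and registry are valid.
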(event `self.ReceiveBeginPlay`
  (`self.Handle Begin Play`))

(event `self.ReceiveEndPlay`
  (params (EndPlayReason :type "EEndPlayReason Enum" :default "Destroyed"))
  (`self.Unregister Marker`))

(fn `Handle Begin Play`
  (`self.On Registered Updated`))

(fn `On Registered Updated`
  (if (`self.Is Registered`)
    (`self.Register Marker`)
    (else
      (`self.Unregister Marker`))))

(fn `OnRep_Is Registered`
  (`self.On Registered Updated`))

(fn `Register Marker`
  (bind _returnvalue (`GameplayStatics.GetPlayerController` 0))
  (bind _returnvalue_2 (`PlayerController.GetHUD` _returnvalue))
  (bind _returnvalue_3 (`Actor.GetComponentByClass` _returnvalue_2 "/Game/Primer/Primer_Markers/BP_MarkerRegistry.BP_MarkerRegistry_C"))
  (`/Engine/EditorBlueprintResources/StandardMacros.IsValid` _returnvalue
    (:`Is Valid`
      (if (`Controller.IsLocalController` _returnvalue)
        (`/Engine/EditorBlueprintResources/StandardMacros.IsValid` _returnvalue_2
          (:`Is Valid`
            (`/Engine/EditorBlueprintResources/StandardMacros.IsValid` _returnvalue_3
              (:`Is Valid`
                (`/Game/Primer/Primer_Markers/BP_MarkerRegistry.Register Marker` _returnvalue_3 self)))))))))

(fn `Unregister Marker`
  (bind _returnvalue (`GameplayStatics.GetPlayerController` 0))
  (bind _returnvalue_2 (`PlayerController.GetHUD` _returnvalue))
  (bind _returnvalue_3 (`Actor.GetComponentByClass` _returnvalue_2 "/Game/Primer/Primer_Markers/BP_MarkerRegistry.BP_MarkerRegistry_C"))
  (`/Engine/EditorBlueprintResources/StandardMacros.IsValid` _returnvalue
    (:`Is Valid`
      (if (`Controller.IsLocalController` _returnvalue)
        (`/Engine/EditorBlueprintResources/StandardMacros.IsValid` _returnvalue_2
          (:`Is Valid`
            (`/Engine/EditorBlueprintResources/StandardMacros.IsValid` _returnvalue_3
              (:`Is Valid`
                (`/Game/Primer/Primer_Markers/BP_MarkerRegistry.Unregister Marker` _returnvalue_3 self)))))))))