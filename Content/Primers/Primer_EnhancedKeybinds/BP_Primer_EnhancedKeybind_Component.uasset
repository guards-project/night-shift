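; Component, meant for the HUD so it runs only locally, that persists and restores player keybinds for an Enhanced Input mapping context.
; On BeginPlay it loads SaveGame_Keybinds from its slot, creating a fresh one if none exists and deleting unreadable saves first.
; A successful load unmaps InputContext and rebuilds each saved mapping, including triggers, modifiers and player-mappable options.
; A separate Save function writes the keybind object back to the slot.
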(event `self.ReceiveBeginPlay`
  ;[1 1 1] attach to HUD = only launch locally
  (`self.Init Save`))

(fn `Apply Saved Keybinds`
  (bind _input_context (`self.Input Context`)
    (:`then`
      (`InputMappingContext.UnmapAll` _input_context)
      (for (_array_element _array_index) (`/Game/Primers/Primer_EnhancedKeybinds/SaveGame_Keybinds.Mappings` (`self.Keybind Save`))
        (`self.Input Context`
          (:`then`
            (bind (_playermappableoptions _triggers _modifiers _action _key _bisplayermappable) (break `EnhancedActionKeyMapping` _array_element))
            (bind _returnvalue (`InputMappingContext.MapKey` _input_context _action _key))
            (bind _structout (setmembers `EnhancedActionKeyMapping` :`StructRef` _returnvalue :`PlayerMappableOptions` _playermappableoptions :`Triggers` _triggers :`Modifiers` _modifiers :`Action` _action :`Key` _key :`bIsPlayerMappable` _bisplayermappable))
            (`KismetArrayLibrary.Array_Set` (`InputMappingContext.Mappings` (`self.Input Context`)) _array_index _structout true))
          (:`else`))))
    (:`else`)))

(fn `Init Save`
  (bind _returnvalue (`GameplayStatics.DoesSaveGameExist` (`self.Slot Name`)))
  (if _returnvalue
    (bind _returnvalue_2 (`GameplayStatics.LoadGameFromSlot` (`self.Slot Name`)))
    (`/Engine/EditorBlueprintResources/StandardMacros.IsValid` _returnvalue_2
      (:`Is Valid`
        (bind _assave_game_keybinds (cast `/Game/Primers/Primer_EnhancedKeybinds/SaveGame_Keybinds` _returnvalue_2)
          (:`then`
            (set `self.Keybind Save` _assave_game_keybinds)
            (`self.Apply Saved Keybinds`))
          (:`CastFailed`
            (`GameplayStatics.DeleteGameInSlot` (`self.Slot Name`) :!label _label)
            (bind _returnvalue_3 (`GameplayStatics.CreateSaveGameObject` "/Game/Primers/Primer_EnhancedKeybinds/SaveGame_Keybinds.SaveGame_Keybinds_C" :!label _label_2))
            (set `self.Keybind Save` _returnvalue_3))))
      (:`Is Not Valid`
        (goto _label)))
    (else
      (goto _label_2))))

(fn `Save`
  (`GameplayStatics.SaveGameToSlot` (`self.Keybind Save`) (`self.Slot Name`)))