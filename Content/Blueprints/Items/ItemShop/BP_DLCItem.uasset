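; BP_DLCItem is an interactable display item that gives local players its item if they own the Vanguard DLC, otherwise opens the DLC page.
; A child actor of ItemClass supplies the preview, interact box and highlight meshes, with collision disabled at BeginPlay.
; Without the DLC, the prompt switches to a basic "Vanguard" widget.
; Interaction is blocked when the same weapon is equipped without room for another default ammo load.
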(event `self.ReceiveBeginPlay`
  (`self.Disable Item Collision`)
  (`KismetSystemLibrary.Delay` 0.2)
  (`self.Update DLC Text`))

(event `Disable Item Collision`
  (bind _childactor (`ChildActorComponent.ChildActor` (`self.Item`))
    (:`then`
      (`self.SetActorEnableCollision` _childactor false))
    (:`else`
      (`KismetSystemLibrary.Delay` 0.2)
      (`self.Disable Item Collision`))))

(event `/Game/Primer/Primer_Interaction/BPI_Interact.Execute Interact`
  (params (User :type "Controller Object Reference"))
  (`parent.Execute Interact` User)
  (if (`Controller.IsLocalPlayerController` User)
    (if (`/Game/_Guards/OnlineSubsystem/BPFL_OnlineSubsystem.Has Vanguard DLC`)
      (bind _asbp_character_template (cast `/Game/Blueprints/Core/BP_Character_Template` (`Controller.K2_GetPawn` User)))
      (`/Game/Blueprints/Items/BP_Inventory_Component.Server Give Item` (`/Game/Blueprints/Core/BP_Character_Template.BP_Inventory_Component` _asbp_character_template) (`|ConvertAsset` (`self.Item Class`)))
      (else
        (`/Game/_Guards/OnlineSubsystem/BPFL_OnlineSubsystem.Open Vanguard DLC Page`)))))

(event `/Game/Primer/Primer_Interaction/BPI_Interact.Stop Focus`)

(fn `Can Pickup`
  (returns (Allow :type Boolean))
  (bind _returnvalue (`GameplayStatics.GetPlayerPawn` 0))
  (`/Engine/EditorBlueprintResources/StandardMacros.IsValid` _returnvalue
    (:`Is Valid`
      (bind _item (message `/Game/Blueprints/Core/BPI_Character.Get Current Equipped Item` _returnvalue))
      (`/Engine/EditorBlueprintResources/StandardMacros.IsValid` _item
        (:`Is Valid`
          (if (== (`self.Item Class`) (`GameplayStatics.GetObjectClass` _item))
            (bind _returnvalue_2 (`self.GetComponentByClass` _item "/Game/Blueprints/Items/BP_ItemAmmo.BP_ItemAmmo_C"))
            (`/Engine/EditorBlueprintResources/StandardMacros.IsValid` _returnvalue_2
              (:`Is Valid`
                (return (<= (+ (`/Game/Blueprints/Items/BP_ItemAmmo.Ammo` _returnvalue_2) (`/Game/Blueprints/Items/BP_ItemAmmo.Default Ammo` _returnvalue_2)) (`/Game/Blueprints/Items/BP_ItemAmmo.Max Ammo` _returnvalue_2))))
              (:`Is Not Valid`
                (return true)))
            (else
              (return true))))
        (:`Is Not Valid`
          (return true))))
    (:`Is Not Valid`
      (return false))))

(fn `Get Can Interact`
  (returns (ReturnValue :type Boolean))
  (return (`self.Can Pickup`)))

(fn `Get Highlight Meshes`
  (returns (Array :type "Array of PrimitiveComponent Object Reference"))
  (bind _childactor (`ChildActorComponent.ChildActor` (`self.Item`)))
  (`/Engine/EditorBlueprintResources/StandardMacros.IsValid` _childactor
    (:`Is Valid`
      (bind _asbp_item (cast `/Game/Blueprints/Items/BP_Item` _childactor))
      (return (`/Game/Blueprints/Items/BP_Item.Get Highlight Meshes` _asbp_item)))
    (:`Is Not Valid`
      (return (`|MakeArray` null :!type "PrimitiveComponent Object Reference")))))

(fn `Update DLC Text`
  (if (not (`/Game/_Guards/OnlineSubsystem/BPFL_OnlineSubsystem.Has Vanguard DLC`))
    (set `self.Interact Text` "Vanguard")
    (set `self.Interact Widget Class` "/Game/Primer/Primer_Interaction/UI/W_Interact_Basic.W_Interact_Basic_C")))

(fn `Update Interact Bounds`
  (bind _box (`self.Box`))
  (bind _childactor (`ChildActorComponent.ChildActor` (`self.Item`))
    (:`then`
      (bind _asbp_item (cast `/Game/Blueprints/Items/BP_Item` _childactor))
      (bind _interactbox (`/Game/Blueprints/Items/BP_Item.InteractBox` _asbp_item))
      (`BoxComponent.SetBoxExtent` _box (`BoxComponent.BoxExtent` _interactbox) true)
      (`SceneComponent.K2_SetRelativeTransform` _box (`SceneComponent.GetRelativeTransform` _interactbox) false false))
    (:`else`)))

(fn `UserConstructionScript`
  (`parent.UserConstructionScript`)
  (`ChildActorComponent.SetChildActorClass` (`self.Item`) (`self.Item Class`))
  (`self.Update Interact Bounds`))