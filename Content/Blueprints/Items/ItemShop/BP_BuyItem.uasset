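; Interactable shop pickup that displays an item as a child actor and sells it for coins.
; The preview has collision disabled and lends its scaled interact box and highlight meshes.
; Focus caches affordability and district unlock from the player save; interaction also requires ammo room when the same item is equipped.
; On purchase, authority gives the item to the buyer's inventory while the local controller deducts coins from its save.
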(event `self.ReceiveBeginPlay`
  (`self.Configure Item`))

(event `Configure Item`
  (bind _childactor (`ChildActorComponent.ChildActor` (`self.Item`))
    (:`then`
      (`self.SetActorEnableCollision` _childactor false)
      (`self.Update Highlight`))
    (:`else`
      (`KismetSystemLibrary.Delay` 0.2)
      (`self.Configure Item`))))

(event `/Game/Primer/Primer_Interaction/BPI_Interact.Start Focus`
  (`|ExecutionSequence`
    (:`then_0`
      (`/Engine/EditorBlueprintResources/StandardMacros.Can Execute Cosmetic Events`
        (:`True`
          (`self.Cache Can Afford`)
          (`self.Cache Unlocked`))))
    (:`then_1`
      (`parent.Start Focus`))))

(event `/Game/Primer/Primer_Interaction/BPI_Interact.Execute Interact`
  (params (User :type "Controller Object Reference"))
  (`parent.Execute Interact` User)
  (`|ExecutionSequence`
    (:`then_0`
      (`/Engine/EditorBlueprintResources/ActorMacros.Switch Has Authority`
        (:`Authority`
          (bind _asbp_character_template (cast `/Game/Blueprints/Core/BP_Character_Template` (`Controller.K2_GetPawn` User)))
          (`/Game/Blueprints/Items/BP_Inventory_Component.Server Give Item` (`/Game/Blueprints/Core/BP_Character_Template.BP_Inventory_Component` _asbp_character_template) (`|ConvertAsset` (`self.Item Class`))))))
    (:`then_1`
      (if (`Controller.IsLocalPlayerController` User)
        (bind _player_save (`/Game/Blueprints/Core/BPFL_Guards.Get Player Save`))
        (`/Game/Blueprints/Core/PlayerSave/SaveGame_Player.Edit Coins` _player_save (* (defaults `Object` (`self.Item Class`)) -1) "Buy Item")
        (`self.Cache Can Afford`)))))

(event `/Game/Primer/Primer_Interaction/BPI_Interact.Stop Focus`
  (`self.Update Highlight`))

(fn `Cache Can Afford`
  (bind _player_save (`/Game/Blueprints/Core/BPFL_Guards.Get Player Save`))
  (`/Engine/EditorBlueprintResources/StandardMacros.IsValid` _player_save
    (:`Is Valid`
      (bind _output_get (set `self.Can Afford` (>= (`/Game/Blueprints/Core/PlayerSave/SaveGame_Player.Coins` _player_save) (defaults `Object` (`self.Item Class`)))))
      (`KismetSystemLibrary.PrintString` (`KismetStringLibrary.Conv_BoolToString` _output_get)))))

(fn `Cache Unlocked`
  (bind _player_save (`/Game/Blueprints/Core/BPFL_Guards.Get Player Save`))
  (set `self.Unlocked` (>= (`/Game/Blueprints/Core/PlayerSave/SaveGame_Player.Highest District Played` _player_save) (`self.District Lock`))))

(fn `Can Pickup`
  (returns (Allow :type Boolean))
  (bind _returnvalue (`GameplayStatics.GetPlayerPawn` 0))
  (`/Engine/EditorBlueprintResources/StandardMacros.IsValid` _returnvalue
    (:`Is Valid`
      (bind _item (message `/Game/Blueprints/Core/BPI_Character.Get Current Equipped Item` _returnvalue))
      (`/Engine/EditorBlueprintResources/StandardMacros.IsValid` _item
        (:`Is Valid`
          (if (== (`self.Item Class`) (`GameplayStatics.GetObjectClass` _item))
            (bind _returnvalue_2 (`self.GetComponentByClass` _item "/Game/Blueprints/Items/BP_ItemAmmo.BP_ItemAmmo_C"))
            (`/Engine/EditorBlueprintResources/StandardMacros.IsValid` _returnvalue_2
              (:`Is Valid`
                (return (<= (+ (`/Game/Blueprints/Items/BP_ItemAmmo.Ammo` _returnvalue_2) (`/Game/Blueprints/Items/BP_ItemAmmo.Default Ammo` _returnvalue_2)) (`/Game/Blueprints/Items/BP_ItemAmmo.Max Ammo` _returnvalue_2))))
              (:`Is Not Valid`
                (return true)))
            (else
              (return true))))
        (:`Is Not Valid`
          (return true))))
    (:`Is Not Valid`
      (return false))))

(fn `Get Can Interact`
  (returns (ReturnValue :type Boolean))
  (return (and (`self.Can Afford`) (`self.Unlocked`) (`self.Can Pickup`))))

(fn `Get Highlight Meshes`
  (returns (Array :type "Array of PrimitiveComponent Object Reference"))
  (bind _childactor (`ChildActorComponent.ChildActor` (`self.Item`)))
  (`/Engine/EditorBlueprintResources/StandardMacros.IsValid` _childactor
    (:`Is Valid`
      (bind _asbp_item (cast `/Game/Blueprints/Items/BP_Item` _childactor))
      (return (`/Game/Blueprints/Items/BP_Item.Get Highlight Meshes` _asbp_item)))
    (:`Is Not Valid`
      (return (`|MakeArray` null :!type "PrimitiveComponent Object Reference")))))

(fn `Update Highlight`
  (if (not (`self.Show Highlight`))
    (bind _asbp_item (cast `/Game/Blueprints/Items/BP_Item` (`ChildActorComponent.ChildActor` (`self.Item`))))
    (`PrimitiveComponent.SetRenderCustomDepth` (`/Game/Blueprints/Items/BP_Item.Item Mesh` _asbp_item) false)))

(fn `Update Interact Bounds`
  (bind _box (`self.Box`))
  (bind _childactor (`ChildActorComponent.ChildActor` (`self.Item`))
    (:`then`
      (bind _asbp_item (cast `/Game/Blueprints/Items/BP_Item` _childactor))
      (bind _interactbox (`/Game/Blueprints/Items/BP_Item.InteractBox` _asbp_item))
      (`BoxComponent.SetBoxExtent` _box (* (`BoxComponent.BoxExtent` _interactbox) (`self.Bound Scale`)) true)
      (`SceneComponent.K2_SetRelativeTransform` _box (`SceneComponent.GetRelativeTransform` _interactbox) false false))
    (:`else`)))

(fn `UserConstructionScript`
  (`parent.UserConstructionScript`)
  (`ChildActorComponent.SetChildActorClass` (`self.Item`) (`self.Item Class`))
  (`self.Update Interact Bounds`))