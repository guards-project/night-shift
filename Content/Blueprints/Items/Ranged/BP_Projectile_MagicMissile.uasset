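; Magic missile projectile that extends a parent projectile class, which supplies the base hit behavior.
; On hit it deactivates its fire trail particle and calls the parent handler.
; When it takes point damage, it executes a hit gameplay cue on the damage causer and destroys itself.
; An unconnected, authority-only branch that would spawn and detonate a Molotov item at its location never runs.
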(event `self.On Hit Event`
  (params (ThisComponent :type "PrimitiveComponent Object Reference") (OtherActor :type "Actor Object Reference") (OtherComp :type "PrimitiveComponent Object Reference") (Hit :type "HitResult Structure (by ref)"))
  (`ActorComponent.Deactivate` (`self.P_Trail_Fire`))
  (`parent.On Hit Event` ThisComponent OtherActor OtherComp Hit))

(event `self.ReceivePointDamage`
  (params (Damage :type "Float (single-precision)") (DamageType :type "DamageType Object Reference") (HitLocation :type "Vector Structure") (HitNormal :type "Vector Structure") (HitComponent :type "PrimitiveComponent Object Reference") (BoneName :type Name) (ShotFromDirection :type "Vector Structure") (InstigatedBy :type "Controller Object Reference") (DamageCauser :type "Actor Object Reference") (HitInfo :type "HitResult Structure (by ref)"))
  (`GameplayCueFunctionLibrary.ExecuteGameplayCueOnActor` DamageCauser (`self.Hit Cue`) (`self.Create Cue Params` HitInfo))
  (`self.K2_DestroyActor`))

(fn `UserConstructionScript`
  (`parent.UserConstructionScript`))