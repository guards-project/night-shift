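; Bolt projectile that sticks into whatever it hits, can pin killed characters to surfaces, and offers a pickup prompt with a focus outline.
; On the server, a lethal hit with a predicted surface ahead spawns a physics constraint that carries the body along, removed on revival or bolt destruction.
; Other hits set a replicated attachment to a bone or component, whose OnRep disables movement and overlaps; fractured targets destroy the bolt.
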(event `self.ReceiveDestroyed`
  (`parent.ReceiveDestroyed`)
  (for _array_element (`self.Constraint`)
    (`/Engine/EditorBlueprintResources/StandardMacros.IsValid` _array_element
      (:`Is Valid`
        (`self.Debug Projectile` (`KismetStringLibrary.Concat_StrStr` "Destroy Constraint " (`KismetSystemLibrary.GetDisplayName` _array_element)))
        (`self.K2_DestroyActor` _array_element)))))

(event `/Game/Primer/Primer_Interaction/BPI_Interact.Start Focus`
  (`PrimitiveComponent.SetRenderCustomDepth` (`self.StaticMesh`) true))

(event `/Game/Primer/Primer_Interaction/BPI_Interact.Stop Focus`
  (`PrimitiveComponent.SetRenderCustomDepth` (`self.StaticMesh`) false))

(fn `Deal Damage`
  (params (`Damaged Actor` :type "Actor Object Reference") (`Other Comp` :type "PrimitiveComponent Object Reference") (Hit :type "HitResult Structure (by ref)"))
  (locals (`L Bone` :type Name) (`L Character` :type "/Game/Blueprints/Core/BP_Character_Template Object Reference") (`L Hit` :type "HitResult Structure"))
  (bind _l_character (`local.L Character`))
  (bind _returnvalue_location (`KismetMathLibrary.BreakTransform` (`SceneComponent.GetSocketTransform` (`local.Other Comp`) (`local.L Bone`) "RTS_World")))
  (bind (_bblockinghit _binitialoverlap _time _distance _location _impactpoint _normal _impactnormal _physmat _hitactor _hitcomponent _hitbonename _bonename) (`GameplayStatics.BreakHitResult` (`local.Hit`)))
  (set `local.L Hit` Hit)
  (`self.Debug Projectile` "Damage Override Started (attach)")
  (`|ExecutionSequence`
    (:`then_0`
      (`/Engine/EditorBlueprintResources/ActorMacros.Switch Has Authority`
        (:`Authority`
          ;[1 1 1] Can Attach
          (`/Engine/EditorBlueprintResources/StandardMacros.IsValid` (`self.GetAttachParentActor`)
            (:`Is Valid`
              (`KismetSystemLibrary.PrintString` "Exit Attach - Found Attached Parent")
              (`self.Disable Overlaps`)
              (`self.Disable Movement`))
            (:`Is Not Valid`
              (bind _asbp_character_template (cast `/Game/Blueprints/Core/BP_Character_Template` (`local.Damaged Actor`))
                (:`then`
                  (set `local.L Character` _asbp_character_template)
                  ;[1 1 1] Attach to Dead Character - keep flying
                  (if (`self.Can Pin`)
                    (if (and (<= (- (`GSCCoreComponent.GetHealth` (`/Game/Blueprints/Core/BP_Character_Template.GSCCore` _l_character)) (`self.Get Damage` (`local.Other Comp`) (`local.Hit`))) 0.0) (== (`KismetArrayLibrary.Array_Length` (`/Game/Blueprints/Core/BP_Character_Template.Constraints` _l_character)) 0) (`self.Predict Wall Pin` (`local.Damaged Actor`)))
                      (`self.Set Moving Attachment` (`local.L Character`) (`local.Hit`))
                      (else
                        ;[1 1 1] Attach to living character - snap to nearest bone
                        (bind _output_get (set `local.L Bone` (select `bool` (== _bonename "None") :`false` _bonename :`true` _hitbonename) :!label _label))
                        (if (== _output_get "None")
                          ;;[1 1 1] Nearest Bone
                          (bind _asskeletal_mesh_component (cast `SkeletalMeshComponent` (`local.Other Comp`))
                            (:`then`
                              (bind (_bonelocation _returnvalue) (`SkinnedMeshComponent.FindClosestBone_K2` _asskeletal_mesh_component (`.Location` (`GameplayStatics.BreakHitResult` (`local.Hit`))) 0.0 true))
                              (set `local.L Bone` (select `bool` (== _returnvalue "None") :`false` _returnvalue :`true` "pelvis"))
                              (`self.Set Static Attachment` (make `/Game/Blueprints/Items/Ranged/F_Attach` (`local.Other Comp`) (`local.L Bone`) (`KismetMathLibrary.MakeRelativeTransform` (`KismetMathLibrary.MakeTransform` _returnvalue_location (`self.K2_GetActorRotation`)) (`SceneComponent.GetSocketTransform` (`local.Other Comp`) (`local.L Bone`) "RTS_World"))) :!label _label_2))
                            (:`CastFailed`
                              (`self.K2_DestroyActor`)))
                          (else
                            (goto _label_2)))))
                    (else
                      (goto _label))))
                (:`CastFailed`
                  ;[1 1 1] Attach Non Character
                  (bind _asbp_fracture_actor (cast `/Game/Blueprints/Fracture/FractureCore/BP_FractureActor` (`local.Damaged Actor`))
                    (:`then`
                      (if (not (`/Game/Blueprints/Fracture/FractureCore/BP_FractureActor.Is Fractured` _asbp_fracture_actor))
                        (`self.Debug Projectile` (`KismetStringLibrary.Concat_StrStr` "Init attachment to non-fractured actor:  " (`KismetSystemLibrary.GetDisplayName` _asbp_fracture_actor)) :!label _label_3)
                        (`self.Set Static Attachment` (make `/Game/Blueprints/Items/Ranged/F_Attach` (`local.Other Comp`) "None" (`KismetMathLibrary.MakeRelativeTransform` (`self.GetTransform`) (`self.GetTransform` (`local.Damaged Actor`)))))
                        (else
                          (`self.Debug Projectile` "Target Fractured, Destroy Bolt")
                          (`self.K2_DestroyActor`))))
                    (:`CastFailed`
                      (goto _label_3))))))))))
    (:`then_1`
      (`self.Debug Projectile` "Damage Override Finished (attach)")
      (`parent.Deal Damage` (`local.Damaged Actor`) (`local.Other Comp`) (`local.L Hit`))
      (return))))

(fn `Disable Overlaps`
  (bind _root_attachment_component (break `/Game/Blueprints/Items/Ranged/F_Attach` (`self.Root Attachment`)))
  (bind _root_attachment_component_2 (break `/Game/Blueprints/Items/Ranged/F_Attach` (`self.Root Attachment`)))
  (`parent.Disable Overlaps`)
  ;[1 1 1] Ignore when moving
  (`/Engine/EditorBlueprintResources/StandardMacros.IsValid` _root_attachment_component
    (:`Is Valid`
      (`PrimitiveComponent.IgnoreActorWhenMoving` (`self.Sphere`) (`ActorComponent.GetOwner` _root_attachment_component) true)
      (`PrimitiveComponent.IgnoreActorWhenMoving` _root_attachment_component_2 self true)
      (`self.Debug Projectile` "+Ignore owner"))))

(fn `Get Always Show Widget`
  (returns (`Always Show` :type Boolean))
  (return false))

(fn `Get Interact Distance`
  (returns (Distance :type "Float (double-precision)"))
  (return 250.0))

(fn `Get Interact Duration`
  (returns (Duration :type "Float (double-precision)"))
  (return 0.0))

(fn `Get Interact Text`
  (returns (Text :type Text))
  (return "Pickup Bolt"))

(fn `Get Interact Widget Class`
  (returns (`Widget Class` :type "/Game/Primer/Primer_Interaction/UI/W_Interact_Master Soft Class Reference"))
  (return "/Game/Primer/Primer_Interaction/UI/W_Interact_Basic.W_Interact_Basic_C"))

(fn `Get Modified Bone`
  (params (InBone :type Name) (InMesh :type "SkinnedMeshComponent Object Reference"))
  (returns (OutBone :type Name))
  (bind (_bonelocation _returnvalue) (`SkinnedMeshComponent.FindClosestBone_K2` InMesh (`self.K2_GetActorLocation` (`self.GetOwner`)) 0.0 true))
  ;[1 1 1] Fixes the floatying ragdoll bug in which a NULL bone would be attached to, causing the body to float.
  (if (or (== InBone "None") (== InBone "None"))
    (return (select `bool` (== _returnvalue "None") :`false` _returnvalue :`true` "pelvis"))
    (else
      (return (`local.InBone`)))))

(fn `On Attached Destroyed`
  (params (DestroyedActor :type "Actor Object Reference"))
  (`self.K2_DestroyActor`))

(fn `On Attached Fractured`
  (params (Actor :type "/Game/Blueprints/Fracture/FractureCore/BP_FractureActor Object Reference"))
  (`self.K2_DestroyActor`))

(fn `On Attachment Updated`
  (bind (_root_attachment_component _root_attachment_bone _root_attachment_relativetransform) (break `/Game/Blueprints/Items/Ranged/F_Attach` (`self.Root Attachment`)))
  (bind (_component _bone) (break `/Game/Blueprints/Items/Ranged/F_Attach` (`self.Root Attachment`)))
  (`self.Debug Projectile` (`KismetStringLibrary.Concat_StrStr` "Attachment Updated: " (`KismetSystemLibrary.GetDisplayName` (`.Component_16_7179BA4B403648FB10CC738584E38CE8` (break `/Game/Blueprints/Items/Ranged/F_Attach` (`self.Root Attachment`))))))
  ;[1 1 1] Become static (don't cause overlaps, only interactable)
  (`/Engine/EditorBlueprintResources/StandardMacros.IsValid` (`.Component_16_7179BA4B403648FB10CC738584E38CE8` (break `/Game/Blueprints/Items/Ranged/F_Attach` (`self.Root Attachment`)))
    (:`Is Valid`
      (`self.Sphere`
        (:`then`
          (`self.Disable Overlaps`)
          (`self.Disable Movement`)
          ;[1 1 1] Attach after disabling
          (`self.K2_AttachToComponent` _component _bone "SnapToTarget" "KeepWorld" "KeepWorld")
          (`self.K2_SetActorRelativeTransform` _root_attachment_relativetransform))
        (:`else`)))))

(fn `On Target Revived`
  (params (Actor :type "/Game/Blueprints/Core/BP_Character_Template Object Reference"))
  (bind (_arrayindex _arrayelement) (`/Engine/EditorBlueprintResources/StandardMacros.ReverseForEachLoop` (`self.Constraint`))
    (:`LoopBody`
      (`/Engine/EditorBlueprintResources/StandardMacros.IsValid` _arrayelement
        (:`Is Valid`
          (`self.K2_DestroyActor` _arrayelement)
          (`KismetArrayLibrary.Array_Remove` (`self.Constraint`) _arrayindex))))))

(fn `OnRep_Root Attachment`
  (`self.On Attachment Updated`))

(fn `Predict Wall Pin`
  (params (Ignore :type "Actor Object Reference"))
  (returns (Allow :type Boolean))
  ;[1 1 1] If the bolt wont pin the player to a surface, then die in place
  ; Solves an issues where players are pinned and thrown outside the map
  ; Only check for player, i.e. enemies always fly
  (bind (_outhit _outpathpositions _outlasttracedestination _returnvalue) (`GameplayStatics.Blueprint_PredictProjectilePath_ByTraceChannel` (`self.K2_GetActorLocation`) (`self.GetVelocity`) true (`SphereComponent.SphereRadius` (`self.Sphere`)) "ECC_Visibility" true (`|MakeArray` Ignore self :!type "Actor Object Reference") "None" 5.0))
  (return _returnvalue))

(fn `Set Moving Attachment`
  (params (`In Character` :type "/Game/Blueprints/Core/BP_Character_Template Object Reference") (Hit :type "HitResult Structure (by ref)"))
  (bind (_bblockinghit _binitialoverlap _time _distance _location _impactpoint _normal _impactnormal _physmat _hitactor _hitcomponent _hitbonename) (`GameplayStatics.BreakHitResult` (`local.Hit`)))
  (`self.Debug Projectile` (`KismetStringLibrary.Concat_StrStr` "attach to dead character and continue flying" (`KismetSystemLibrary.GetDisplayName` (`local.In Character`))))
  (`/Game/Blueprints/Core/BP_Character_Template.Remove Death Constraint` (`local.In Character`))
  (add `/Game/Blueprints/Core/BP_Character_Template.OnRevived` (`local.In Character`) (`|CreateDelegate` :!event `On Target Revived`)) ; remove physics constraints after revival
  (bind _returnvalue (`|SpawnActorFromClass` "/Game/Blueprints/Items/Ranged/BP_Constraint.BP_Constraint_C" (`self.GetTransform`) "AlwaysSpawn" "OverrideRootScale" self (make `/Game/Blueprints/Items/Ranged/F_Constraint` _hitcomponent (`self.Get Modified Bone` _hitbonename (`Character.Mesh` (`local.In Character`))) (`self.Sphere`)) (`self.Debug`) null)) ; spawn a constraint that constrains the character mesh to this projectile
  (`KismetArrayLibrary.Array_Add` (`self.Constraint`) _returnvalue)
  (`self.K2_AttachToActor` _returnvalue self "None" "SnapToTarget" "SnapToTarget" "KeepRelative" true) ; attach the constraint to this projectile so they move together
  (`/Game/Blueprints/Core/BP_Character_Template.Track Constraint` (`local.In Character`) _returnvalue))

(fn `Set Static Attachment`
  (params (`In Attachment` :type "/Game/Blueprints/Items/Ranged/F_Attach Structure"))
  (bind _returnvalue (`self.GetAttachParentActor`))
  (bind _sphere (`self.Sphere`))
  (bind (_component _bone) (break `/Game/Blueprints/Items/Ranged/F_Attach` (`local.In Attachment`)))
  (bind (_component_2 _bone_2) (break `/Game/Blueprints/Items/Ranged/F_Attach` (`local.In Attachment`)))
  (`PrimitiveComponent.SetCollisionResponseToChannel` _sphere "ECC_WorldStatic" "ECR_Ignore")
  (`PrimitiveComponent.SetCollisionResponseToChannel` _sphere "ECC_GameTraceChannel2" "ECR_Ignore") ; don't break crates
  (`self.Debug Projectile` (`KismetStringLibrary.Concat_StrStr` "Set Attacment to bone: " (`KismetSystemLibrary.GetDisplayName` _component) " Optional Bone: " (`KismetStringLibrary.Conv_NameToString` _bone)))
  (set `self.Root Attachment` (`local.In Attachment`))
  ;[1 1 1] Destroy self when attach target is destroyed or fractured
  (`/Engine/EditorBlueprintResources/StandardMacros.IsValid` _returnvalue
    (:`Is Valid`
      (add `self.OnDestroyed` _returnvalue (`|CreateDelegate` :!event `On Attached Destroyed`))
      (bind _asbp_fracture_actor (cast `/Game/Blueprints/Fracture/FractureCore/BP_FractureActor` _returnvalue)
        (:`then`
          (add `/Game/Blueprints/Fracture/FractureCore/BP_FractureActor.Fractured` _asbp_fracture_actor (`|CreateDelegate` :!event `On Attached Fractured`)))
        (:`CastFailed`
          (`/Engine/EditorBlueprintResources/StandardMacros.IsValid` _component_2
            (:`Is Valid`
              (if (`self.ActorHasTag` (`ActorComponent.GetOwner` _component_2) "Player")
                (if (== _bone_2 "Head")
                  (`KismetSystemLibrary.K2_SetTimerDelegate` (`|CreateDelegate` :!event `K2_DestroyActor`) 10.0))))))))))

(fn `UserConstructionScript`
  (`parent.UserConstructionScript`))