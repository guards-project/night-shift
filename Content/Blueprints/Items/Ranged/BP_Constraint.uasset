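; Replicated constraint actor that physically binds two components at named bones, filed under ranged items.
; On begin play or replication, it snaps the simulating first component to the actor, offset by its bone, then constrains it and disables some collision responses on Character meshes.
; Timers drive retries after failed setup and periodic checks.
; TestBreaks rebuilds when the bone drifts past a threshold, or destroys the actor if that component is invalid.
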(event `self.ReceiveBeginPlay`
  (`self.Update Constraint`)
  (`KismetSystemLibrary.K2_SetTimerDelegate` (`|CreateDelegate` :!event `Test Breaks`) 1.0 true))

(event `self.ReceiveDestroyed`
  (bind _debug (`self.Debug`))
  (`PhysicsConstraintComponent.SetConstrainedComponents` (`self.PhysicsConstraint`) null "None" null "None")
  (`KismetSystemLibrary.PrintString` "Constraint Destroyed" _debug _debug))

(fn `Get Constraint`
  (returns (Constraint :type "/Game/Blueprints/Items/Ranged/F_Constraint Structure"))
  (return (`self.Constraint`)))

(fn `OnRep_Constraint`
  (`self.Update Constraint`))

(fn `Test Breaks`
  (bind ((`Component1_10_7179BA4B403648FB10CC738584E38CE8` _component1) (`Bone1_7_84C259E146C93A6A2F1EF59296716160` _bone1)) (break `/Game/Blueprints/Items/Ranged/F_Constraint` (`self.Get Constraint`)))
  (bind _returnvalue_location (`KismetMathLibrary.BreakTransform` (`SceneComponent.GetSocketTransform` _component1 _bone1 "RTS_World")))
  (`/Engine/EditorBlueprintResources/StandardMacros.IsValid` _component1
    (:`Is Valid`
      (if (> (`KismetMathLibrary.Vector_Distance` _returnvalue_location (`self.K2_GetActorLocation`)) (`self.Refresh Threshold`))
        (`self.Update Constraint`)))
    (:`Is Not Valid`
      (`self.K2_DestroyActor`))))

(fn `Update Constraint`
  (bind _debug (`self.Debug`))
  (bind _debug_2 (`self.Debug`))
  (bind (_component1 _bone1 _component2 _bone2) (break `/Game/Blueprints/Items/Ranged/F_Constraint` (`self.Get Constraint`)))
  (bind (_component1_2 _bone1_2 _component2_2) (break `/Game/Blueprints/Items/Ranged/F_Constraint` (`self.Get Constraint`)))
  (bind (_component1_3 _bone1_3 _component2_3) (break `/Game/Blueprints/Items/Ranged/F_Constraint` (`self.Get Constraint`)))
  (bind ((`Component1_10_7179BA4B403648FB10CC738584E38CE8` _component1_4) (`Bone1_7_84C259E146C93A6A2F1EF59296716160` _bone1_4)) (break `/Game/Blueprints/Items/Ranged/F_Constraint` (`self.Get Constraint`)))
  (bind ((`Component1_10_7179BA4B403648FB10CC738584E38CE8` _component1_5)) (break `/Game/Blueprints/Items/Ranged/F_Constraint` (`self.Get Constraint`)))
  (bind _returnvalue_location (`KismetMathLibrary.BreakTransform` (`SceneComponent.GetSocketTransform` _component1_4 _bone1_4 "RTS_Component")))
  (if (and (`KismetSystemLibrary.IsValid` _component1_2) (`KismetSystemLibrary.IsValid` _component2_2))
    (if (`SceneComponent.IsAnySimulatingPhysics` _component1_2)
      (`SceneComponent.K2_SetWorldTransform` _component1_5 (`self.GetTransform`) false true)
      (`SceneComponent.K2_AddLocalOffset` _component1_5 (* _returnvalue_location -1) false true)
      (`PhysicsConstraintComponent.SetConstrainedComponents` (`self.PhysicsConstraint`) _component1 _bone1 _component2 _bone2)
      (`KismetSystemLibrary.PrintString` (`KismetStringLibrary.Concat_StrStr` "Constraint Created: " (`KismetSystemLibrary.GetDisplayName` _component1_3) " and " (`KismetSystemLibrary.GetDisplayName` _component2_3)) _debug _debug)
      (`|ExecutionSequence`
        (:`then_0`
          (bind _ascharacter (cast `Character` (`ActorComponent.GetOwner` _component1)))
          (bind _mesh (`Character.Mesh` _ascharacter))
          (`PrimitiveComponent.SetCollisionResponseToChannel` _mesh "ECC_PhysicsBody" "ECR_Ignore")
          (`PrimitiveComponent.SetCollisionResponseToChannel` _mesh "ECC_GameTraceChannel1" "ECR_Ignore"))
        (:`then_1`
          (bind _ascharacter_2 (cast `Character` (`ActorComponent.GetOwner` _component2)))
          (bind _mesh_2 (`Character.Mesh` _ascharacter_2))
          (`PrimitiveComponent.SetCollisionResponseToChannel` _mesh_2 "ECC_PhysicsBody" "ECR_Ignore")
          (`PrimitiveComponent.SetCollisionResponseToChannel` _mesh_2 "ECC_GameTraceChannel1" "ECR_Ignore")))
      (else
        (`KismetSystemLibrary.K2_SetTimerDelegate` (`|CreateDelegate` :!event `Update Constraint`) 0.1 :!label _label)
        (`KismetSystemLibrary.PrintString` "Constriant Failed" _debug_2 _debug_2)))
    (else
      (goto _label))))

(fn `UserConstructionScript`)