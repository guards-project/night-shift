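; Red magic missile projectile for ranged items, a child Blueprint that adds timed homing and fire-trail handling to its parent.
; On BeginPlay the authority starts a timer that later switches off homing and turns on gravity, so the missile drops.
; On hit it deactivates the fire trail, then defers to the parent's hit logic.
; Older hit effect and Molotov explosion logic remains in the graph but is disconnected.
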(event `self.ReceiveBeginPlay`
  (`parent.ReceiveBeginPlay`)
  (`/Engine/EditorBlueprintResources/ActorMacros.Switch Has Authority`
    (:`Authority`
      (`KismetSystemLibrary.K2_SetTimerDelegate` (delegate `Stop Homing`) 5.0))))

(event `Stop Homing`
  (bind _projectilemovement (`self.ProjectileMovement`))
  (set `ProjectileMovementComponent.bIsHomingProjectile` false _projectilemovement)
  (set `ProjectileMovementComponent.ProjectileGravityScale` 1.0 _projectilemovement))

(event `self.On Hit Event`
  (params (ThisComponent :type "PrimitiveComponent Object Reference") (OtherActor :type "Actor Object Reference") (OtherComp :type "PrimitiveComponent Object Reference") (Hit :type "HitResult Structure (by ref)"))
  (`ActorComponent.Deactivate` (`self.P_Trail_Fire`))
  (`parent.On Hit Event` ThisComponent OtherActor OtherComp Hit))

(fn `UserConstructionScript`
  (`parent.UserConstructionScript`))