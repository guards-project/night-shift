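; Base ranged-weapon projectile with configurable speed, gravity and optional homing, which players can pick up to regain ammo.
; Server-side hits and de-duplicated overlaps skip the instigator, apply point damage with a fixed headshot value against non-players, fire a GameplayCue, create noise and optionally destroy it.
; Blocking hits disable sphere overlaps but keep the mesh queryable, so interacting can rearm a held ranged weapon that has spare capacity.
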(event `self.ReceiveBeginPlay`
  (`parent.ReceiveBeginPlay`)
  (`/Engine/EditorBlueprintResources/ActorMacros.Switch Has Authority`
    (:`Authority`
      (`self.MC Sounds`) ; one shot event, not for late joiners
    )))

(event `MC Sounds`
  (`GameplayStatics.PlaySoundAtLocation` (`self.Start Sound`) (`self.K2_GetActorLocation`) (struct) 1.0 1.0 0.0 null null null null)
  (`ActorComponent.Activate` (`self.Fly_Cue`) true))

(event `self.ReceiveHit`
  (params (MyComp :type "PrimitiveComponent Object Reference") (Other :type "Actor Object Reference") (OtherComp :type "PrimitiveComponent Object Reference") (bSelfMoved :type Boolean) (HitLocation :type "Vector Structure") (HitNormal :type "Vector Structure") (NormalImpulse :type "Vector Structure") (Hit :type "HitResult Structure (by ref)"))
  (`self.On Hit Event` MyComp Other OtherComp Hit))

(event `self.Sphere.OnComponentBeginOverlap`
  (params (OverlappedComponent :type "PrimitiveComponent Object Reference") (OtherActor :type "Actor Object Reference") (OtherComp :type "PrimitiveComponent Object Reference") (OtherBodyIndex :type Integer) (bFromSweep :type Boolean) (SweepResult :type "HitResult Structure (by ref)"))
  (`self.On Overlap Event` OverlappedComponent OtherActor OtherComp SweepResult))

(event `Play Damage Cue`
  (params (Target :type "Actor Object Reference") (HitResult :type "HitResult Structure (by ref)"))
  (`GameplayCueFunctionLibrary.ExecuteGameplayCueOnActor` Target (`self.Hit Cue`) (`self.Create Cue Params` HitResult)))

(event `/Game/Primer/Primer_Interaction/BPI_Interact.Execute Interact`
  (params (User :type "Controller Object Reference"))
  (`self.Rearm` User))

(fn `Can Rearm`
  (returns (ReturnValue :type Boolean))
  (locals (`L Ranged Weapon` :type "/Game/Blueprints/Items/Ranged/BP_Item_RangedWeapon Object Reference"))
  (bind _returnvalue (`GameplayStatics.GetPlayerPawn` 0))
  (bind _returnvalue_2 (`self.GetComponentByClass` _returnvalue "/Game/Blueprints/Items/BP_Inventory_Component.BP_Inventory_Component_C"))
  (bind _bp_itemammo (`/Game/Blueprints/Items/Ranged/BP_Item_RangedWeapon.BP_ItemAmmo` (`local.L Ranged Weapon`)))
  (`/Engine/EditorBlueprintResources/StandardMacros.IsValid` _returnvalue
    (:`Is Valid`
      (`/Engine/EditorBlueprintResources/StandardMacros.IsValid` _returnvalue_2
        (:`Is Valid`
          (bind (_item _shield) (`/Game/Blueprints/Items/BP_Inventory_Component.Get Items` _returnvalue_2))
          (`|ExecutionSequence`
            (:`then_0`
              (`/Engine/EditorBlueprintResources/StandardMacros.IsValid` _item
                (:`Is Valid`
                  (bind _asbp_item_ranged_weapon (cast `/Game/Blueprints/Items/Ranged/BP_Item_RangedWeapon` _item))
                  (set `local.L Ranged Weapon` _asbp_item_ranged_weapon))))
            (:`then_1`
              (`/Engine/EditorBlueprintResources/StandardMacros.IsValid` _shield
                (:`Is Valid`
                  (bind _asbp_item_ranged_weapon_2 (cast `/Game/Blueprints/Items/Ranged/BP_Item_RangedWeapon` _shield))
                  (set `local.L Ranged Weapon` _asbp_item_ranged_weapon_2))))
            (:`then_2`
              (return false)))
          (if (and (< (`/Game/Blueprints/Items/BP_ItemAmmo.Ammo` _bp_itemammo) (`/Game/Blueprints/Items/BP_ItemAmmo.Max Ammo` _bp_itemammo)) (or (`KismetMathLibrary.ClassIsChildOf` (`GameplayStatics.GetObjectClass` self) (`/Game/Blueprints/Items/Ranged/BP_Item_RangedWeapon.Projectile Class` (`local.L Ranged Weapon`))) (`KismetMathLibrary.ClassIsChildOf` (`/Game/Blueprints/Items/Ranged/BP_Item_RangedWeapon.Projectile Class` (`local.L Ranged Weapon`)) (`GameplayStatics.GetObjectClass` self))))
            (return true)))))))

(fn `Check Destroy`
  (if (`self.Destroy After Damage`)
    (`self.K2_DestroyActor`)))

(fn `Create Cue Params`
  (params (HitResult :type "HitResult Structure (by ref)"))
  (returns (ReturnValue :type "GameplayCueParameters Structure"))
  (bind (_returnvalue_normalizedmagnitude _returnvalue_rawmagnitude _returnvalue_effectcontext _returnvalue_matchedtagname _returnvalue_originaltag _returnvalue_aggregatedsourcetags _returnvalue_aggregatedtargettags _returnvalue_location _returnvalue_normal _returnvalue_instigator _returnvalue_effectcauser _returnvalue_sourceobject _returnvalue_physicalmaterial _returnvalue_gameplayeffectlevel _returnvalue_abilitylevel _returnvalue_targetattachcomponent) (`AbilitySystemBlueprintLibrary.BreakGameplayCueParameters` (`GameplayCueFunctionLibrary.MakeGameplayCueParametersFromHitResult` HitResult)))
  (bind (_bblockinghit _binitialoverlap _time _distance _location _impactpoint _normal _impactnormal _physmat _hitactor) (`GameplayStatics.BreakHitResult` (`local.HitResult`)))
  (return (`AbilitySystemBlueprintLibrary.MakeGameplayCueParameters` _returnvalue_normalizedmagnitude _returnvalue_rawmagnitude _returnvalue_effectcontext _returnvalue_matchedtagname _returnvalue_originaltag _returnvalue_aggregatedsourcetags _returnvalue_aggregatedtargettags (`self.K2_GetActorLocation`) (`self.GetActorForwardVector`) (`self.Instigator`) self _hitactor (select `bool` (`.bSuccess` (cast `Character` _hitactor :!pure true)) :`false` _returnvalue_physicalmaterial :`true` "/Game/_Guards/Art/Physmats/PhysMat_Flesh.PhysMat_Flesh") _returnvalue_gameplayeffectlevel _returnvalue_abilitylevel _returnvalue_targetattachcomponent true)))

(fn `Deal Damage`
  (params (`Damaged Actor` :type "Actor Object Reference") (`Other Comp` :type "PrimitiveComponent Object Reference") (Hit :type "HitResult Structure (by ref)"))
  (locals (`L Damage` :type "Float (double-precision)" :default 0.0))
  (`self.Play Damage Cue` `Damaged Actor` Hit)
  (set `local.L Damage` (`self.Get Damage` (`local.Other Comp`) Hit))
  (`self.Debug Projectile` (`KismetStringLibrary.Concat_StrStr` "Apply Damage: " (`KismetStringLibrary.Conv_DoubleToString` (`local.L Damage`)) " to: " (`KismetSystemLibrary.GetDisplayName` (`local.Damaged Actor`))))
  (`GameplayStatics.ApplyPointDamage` (`local.Damaged Actor`) (`local.L Damage`) (* (`self.GetVelocity`) -1.0) (`local.Hit`) (`self.GetInstigatorController`) self (`self.Damage Type Class`)) ; todo causer = owner character
  (`/Game/Blueprints/Core/PolygonAI/SenseData/BPFL_Noise.Create Noise` self (`self.K2_GetActorLocation`) (`self.Noise`)))

(fn `Debug Projectile`
  (params (InString :type String))
  (bind _debug (`self.Debug`))
  (`KismetSystemLibrary.PrintString` InString _debug _debug))

(fn `Disable Movement`
  (bind _projectilemovement (`self.ProjectileMovement`))
  (`self.ProjectileMovement`
    (:`then`
      (`MovementComponent.StopMovementImmediately` _projectilemovement)
      (`ProjectileMovementComponent.StopSimulating` _projectilemovement (`GameplayStatics.MakeHitResult` false))
      (`self.Debug Projectile` "Movement Disabled"))
    (:`else`)))

(fn `Disable Overlaps`
  (`PrimitiveComponent.SetCollisionResponseToChannel` (`self.Sphere`) "ECC_GameTraceChannel1" "ECR_Ignore")
  (`PrimitiveComponent.SetCollisionResponseToChannel` (`self.Sphere`) "ECC_PhysicsBody" "ECR_Ignore")
  (`PrimitiveComponent.SetCollisionResponseToChannel` (`self.Sphere`) "ECC_GameTraceChannel2" "ECR_Ignore")
  (`PrimitiveComponent.SetCollisionResponseToChannel` (`self.Sphere`) "ECC_Pawn" "ECR_Ignore")
  (`PrimitiveComponent.SetCollisionEnabled` (`self.StaticMesh`) "QueryOnly") ; allow interact to work
  (`self.Debug Projectile` "Disabled Overlaps"))

(fn `Get Always Show Widget`
  (returns (`Always Show` :type Boolean))
  (return false))

(fn `Get Can Interact`
  (returns (ReturnValue :type Boolean))
  (locals (`L Ranged Weapon` :type "/Game/Blueprints/Items/Ranged/BP_Item_RangedWeapon Object Reference"))
  (bind _returnvalue (`self.Can Rearm`))
  (return _returnvalue))

(fn `Get Damage`
  (params (`In Comp` :type "SceneComponent Object Reference") (`In Hit` :type "HitResult Structure (by ref)"))
  (returns (ReturnValue :type "Float (double-precision)"))
  (bind (_bblockinghit _binitialoverlap _time _distance _location _impactpoint _normal _impactnormal _physmat _hitactor _hitcomponent _hitbonename _bonename) (`GameplayStatics.BreakHitResult` `In Hit`))
  (return (`KismetMathLibrary.SelectFloat` 15.0 (`self.Projectile Damage`) (and (or (<= (`KismetMathLibrary.Vector_Distance` (`.Location` (`GameplayStatics.BreakHitResult` (`local.In Hit`))) (`SceneComponent.GetSocketLocation` (`local.In Comp`) "head")) 20.0) (== _hitbonename "head") (== _bonename "head")) (not (`self.ActorHasTag` (`ActorComponent.GetOwner` (`local.In Comp`)) "Player"))))))

(fn `Get Interact Distance`
  (returns (Distance :type "Float (double-precision)"))
  (return 0.0))

(fn `Get Interact Duration`
  (returns (Duration :type "Float (double-precision)"))
  (return 0.0))

(fn `Get Interact Text`
  (returns (Text :type Text))
  (return ""))

(fn `Get Interact Widget Class`
  (returns (`Widget Class` :type "/Game/Primer/Primer_Interaction/UI/W_Interact_Master Soft Class Reference"))
  (return null))

(fn `On Hit Event`
  (params (ThisComponent :type "PrimitiveComponent Object Reference") (OtherActor :type "Actor Object Reference") (OtherComp :type "PrimitiveComponent Object Reference") (Hit :type "HitResult Structure (by ref)"))
  (`/Engine/EditorBlueprintResources/StandardMacros.IsValid` OtherComp
    (:`Is Valid`
      (`self.Debug Projectile` (`KismetStringLibrary.Concat_StrStr` "Hit " (`KismetSystemLibrary.GetDisplayName` OtherComp)))
      (`self.Disable Overlaps`)
      (`/Engine/EditorBlueprintResources/ActorMacros.Switch Has Authority`
        (:`Authority`
          (if (!= (`local.OtherActor`) (`self.GetInstigator`))
            (`self.Deal Damage` OtherActor OtherComp Hit)
            (`self.Check Destroy`)))))))

(fn `On Overlap Event`
  (params (ThisComponent :type "PrimitiveComponent Object Reference") (OtherActor :type "Actor Object Reference") (OtherComp :type "PrimitiveComponent Object Reference") (Hit :type "HitResult Structure (by ref)"))
  (`/Engine/EditorBlueprintResources/StandardMacros.IsValid` OtherComp
    (:`Is Valid`
      (`self.Debug Projectile` (`KismetStringLibrary.Concat_StrStr` "Overlap  " (`KismetSystemLibrary.GetDisplayName` OtherComp)))
      (`/Engine/EditorBlueprintResources/ActorMacros.Switch Has Authority`
        (:`Authority`
          (if (!= (`local.OtherActor`) (`self.GetInstigator`))
            (bind _returnvalue (`KismetArrayLibrary.Array_AddUnique` (`self.Overlap Cache`) (`local.OtherActor`)))
            (if (>= _returnvalue 0)
              (`self.Deal Damage` OtherActor OtherComp Hit)
              (`self.Check Destroy`))))))))

(fn `Rearm`
  (params (User :type "Controller Object Reference"))
  (locals (`L Ranged Weapon` :type "/Game/Blueprints/Items/Ranged/BP_Item_RangedWeapon Object Reference"))
  (bind _returnvalue (`Controller.K2_GetPawn` User))
  (bind _bp_itemammo (`/Game/Blueprints/Items/Ranged/BP_Item_RangedWeapon.BP_ItemAmmo` (`local.L Ranged Weapon`)))
  (bind _bp_itemammo_2 (`/Game/Blueprints/Items/Ranged/BP_Item_RangedWeapon.BP_ItemAmmo` (`local.L Ranged Weapon`)))
  (`GameplayStatics.PlaySoundAtLocation` (`self.Rearm Sound`) (`self.K2_GetActorLocation`) (struct) 1.0 1.0 0.0 null null null null)
  (`/Engine/EditorBlueprintResources/ActorMacros.Switch Has Authority`
    (:`Authority`
      (`/Engine/EditorBlueprintResources/StandardMacros.IsValid` _returnvalue
        (:`Is Valid`
          (bind (_item _shield) (`/Game/Blueprints/Items/BP_Inventory_Component.Get Items` (`self.GetComponentByClass` _returnvalue "/Game/Blueprints/Items/BP_Inventory_Component.BP_Inventory_Component_C")))
          (`|ExecutionSequence`
            (:`then_0`
              (`/Engine/EditorBlueprintResources/StandardMacros.IsValid` _item
                (:`Is Valid`
                  (bind _asbp_item_ranged_weapon (cast `/Game/Blueprints/Items/Ranged/BP_Item_RangedWeapon` _item))
                  (set `local.L Ranged Weapon` _asbp_item_ranged_weapon))))
            (:`then_1`
              (`/Engine/EditorBlueprintResources/StandardMacros.IsValid` _shield
                (:`Is Valid`
                  (bind _asbp_item_ranged_weapon_2 (cast `/Game/Blueprints/Items/Ranged/BP_Item_RangedWeapon` _shield))
                  (set `local.L Ranged Weapon` _asbp_item_ranged_weapon_2)))))
          (if (< (`/Game/Blueprints/Items/BP_ItemAmmo.Ammo` _bp_itemammo) (`/Game/Blueprints/Items/BP_ItemAmmo.Max Ammo` _bp_itemammo))
            (set `/Game/Blueprints/Items/BP_ItemAmmo.Ammo` (+ (`/Game/Blueprints/Items/BP_ItemAmmo.Ammo` _bp_itemammo_2) 1) _bp_itemammo_2)
            (`self.K2_DestroyActor`) ; pickup
            (return)))))))

(fn `Set Homing Target`
  (params (`In Homing` :type Boolean) (`In Target Component` :type "SceneComponent Object Reference"))
  (bind _projectilemovement (`self.ProjectileMovement`))
  (set `ProjectileMovementComponent.HomingTargetComponent` (`local.In Target Component`) _projectilemovement)
  (set `ProjectileMovementComponent.bIsHomingProjectile` (`local.In Homing`) _projectilemovement))

(fn `UserConstructionScript`
  (bind _projectilemovement (`self.ProjectileMovement`))
  (bind _speed (`self.Speed`))
  (set `ProjectileMovementComponent.InitialSpeed` _speed _projectilemovement)
  (set `ProjectileMovementComponent.MaxSpeed` _speed _projectilemovement)
  (set `ProjectileMovementComponent.ProjectileGravityScale` (`self.Gravity Scale`) _projectilemovement))