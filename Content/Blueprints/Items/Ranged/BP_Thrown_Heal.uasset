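; Thrown healing potion that bursts on impact into a short-lived heal cloud.
; On first hit it hides, and the server briefly enables an overlap sphere that applies GE_HealCloud once per character before destroying the actor.
; Cosmetic-capable instances play smash sound, Niagara burst and red volumetric mist.
; Equipping ignores PhysicsBody collision and, on AI owners, disables death loot and sets their loot spawner to potions, intended as an arrest reward.
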(event `self.On Equipped`
  (params (NewOwner :type "Actor Object Reference"))
  ;[1 1 1] stops flying into sky
  (`parent.On Equipped` NewOwner)
  (`PrimitiveComponent.SetCollisionResponseToChannel` (`self.Item Mesh`) "ECC_PhysicsBody" "ECR_Ignore")
  (bind _asbp_polygon_ai (cast `/Game/Blueprints/Core/PolygonAI/BP_Polygon_AI` NewOwner))
  (set `/Game/Blueprints/Core/PolygonAI/BP_Polygon_AI.Can Spawn Loot On Death` false _asbp_polygon_ai) ; only allow loot potions if you arrest them
  (bind _bp_lootspawner_component_coins (`/Game/Blueprints/Core/PolygonAI/BP_Polygon_AI.BP_LootSpawner_Component_Coins` _asbp_polygon_ai))
  (set `/Game/Blueprints/LootSpawner/BP_LootSpawner_Component.Use DT_Loot` false _bp_lootspawner_component_coins)
  (set `/Game/Blueprints/LootSpawner/BP_LootSpawner_Component.Loot Config` (make `/Game/Blueprints/LootSpawner/F_LootConfig` null (`|MakeArray` (make `/Game/Blueprints/LootSpawner/F_LootSpawnable` "/Game/Blueprints/Items/Ranged/BP_Thrown_Heal.BP_Thrown_Heal_C") :!type "/Game/Blueprints/LootSpawner/F_LootSpawnable Structure") 1.0 3 5) _bp_lootspawner_component_coins))

(event `self.On Unequipped`
  ;[1 1 1] stops flying into sky
  (`parent.On Unequipped`)
  (`PrimitiveComponent.SetCollisionResponseToChannel` (`self.Item Mesh`) "ECC_PhysicsBody" "ECR_Block"))

(event `self.Execute Gameplay Thrown Hit Cue`
  (bind (_bblockinghit _binitialoverlap _time _distance _location) (`GameplayStatics.BreakHitResult` (`self.Last Hit`)))
  (`parent.Execute Gameplay Thrown Hit Cue`)
  (`/Engine/EditorBlueprintResources/StandardMacros.DoOnce` false
    (:`Completed`
      (`self.SetActorHiddenInGame` true)
      (`|ExecutionSequence`
        (:`then_0`
          (`/Engine/EditorBlueprintResources/ActorMacros.Switch Has Authority`
            (:`Authority`
              (`SceneComponent.K2_SetWorldLocation` (`self.Sphere`) (`.Location` (`GameplayStatics.BreakHitResult` (`self.Last Hit`))) false false)
              (`PrimitiveComponent.SetCollisionEnabled` (`self.Sphere`) "QueryOnly")
              (`KismetSystemLibrary.Delay` 0.5)
              (`PrimitiveComponent.SetCollisionEnabled` (`self.Sphere`) "NoCollision")
              (`KismetSystemLibrary.Delay` 1.0)
              (`self.K2_DestroyActor`))))
        (:`then_1`
          (`/Engine/EditorBlueprintResources/StandardMacros.Can Execute Cosmetic Events`
            (:`True`
              (`GameplayStatics.PlaySoundAtLocation` "/Game/_Guards/Audio/Hits/A_BottleSmash_Cue.A_BottleSmash_Cue" (`.Location` (`GameplayStatics.BreakHitResult` (`self.Last Hit`))) (struct) 1.0 1.0 0.0 null null null null)
              (`ActorComponent.Deactivate` (`self.Niagara`))
              (`ActorComponent.Deactivate` (`self.Niagara1`))
              (`NiagaraFunctionLibrary.SpawnSystemAtLocation` "/Game/TrailEffect/Fx/Niagara/NS_HealExplosion.NS_HealExplosion" _location)
              (bind _returnvalue (`|SpawnActorFromClass` "/Game/UltraVolumetrics/Blueprints/BP_UltraVolumetrics_Miff.BP_UltraVolumetrics_Miff_C" (`KismetMathLibrary.MakeTransform` _location) "Undefined" "MultiplyWithRoot" null "NewEnumerator0" 5.0 true 20.0 -1.0 1.0 0.4 (0.5 0.5 1.0) 2.0 1.0 (struct :`R` 0.814847 :`G` 0.021219 :`B` 0.021219 :`A` 1.0) (struct :`R` 0.296875 :`G` 0.007731 :`B` 0.007731 :`A` 1.0) 0.0 0.0 -0.2 0.0 6000.0 1.612889 false 0.0 1.737688 0.180952 0.5 null))
              (`self.SetLifeSpan` _returnvalue 1.0))))))))

(event `self.Sphere.OnComponentBeginOverlap`
  (params (OverlappedComponent :type "PrimitiveComponent Object Reference") (OtherActor :type "Actor Object Reference") (OtherComp :type "PrimitiveComponent Object Reference") (OtherBodyIndex :type Integer) (bFromSweep :type Boolean) (SweepResult :type "HitResult Structure (by ref)"))
  (bind _asbp_character_template (cast `/Game/Blueprints/Core/BP_Character_Template` OtherActor))
  (if (not (`KismetArrayLibrary.Array_Contains` (`self.Applied`) _asbp_character_template))
    (`KismetArrayLibrary.Array_AddUnique` (`self.Applied`) _asbp_character_template)
    (bind _returnvalue (`AbilitySystemBlueprintLibrary.GetAbilitySystemComponent` _asbp_character_template))
    (`AbilitySystemComponent.BP_ApplyGameplayEffectToSelf` _returnvalue "/Game/Blueprints/Items/Interactable/Pickups/GE_HealCloud.GE_HealCloud_C" 6.0 (`AbilitySystemComponent.MakeEffectContext` _returnvalue))))

(fn `UserConstructionScript`
  (`parent.UserConstructionScript`))