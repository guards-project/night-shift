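; Tripwire bolt projectile that, on impact, links to other tripwire bolts within range and knocks out characters crossing the wires, with a velocity-based ragdoll impulse.
; The replicated AttachedWires array's OnRep rebuilds wire components, while the server prunes invalid or out-of-range links.
; Invulnerable characters and those either linked bolt is attached to never trip.
; Bolts survive their attachment's destruction for snapshot compatibility, but not its fracture.
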(event `/Game/Primer/Primer_Interaction/BPI_Interact.Start Focus`
  (`PrimitiveComponent.SetRenderCustomDepth` (`self.StaticMesh`) true))

(event `/Game/Primer/Primer_Interaction/BPI_Interact.Stop Focus`
  (`PrimitiveComponent.SetRenderCustomDepth` (`self.StaticMesh`) false))

(event `self.Wire.OnComponentBeginOverlap`
  (params (OverlappedComponent :type "PrimitiveComponent Object Reference") (OtherActor :type "Actor Object Reference") (OtherComp :type "PrimitiveComponent Object Reference") (OtherBodyIndex :type Integer) (bFromSweep :type Boolean) (SweepResult :type "HitResult Structure (by ref)"))
  (`self.Trip Target` OtherActor SweepResult))

(event `self.Set Static Attachment`
  (params (`In Attachment` :type "/Game/Blueprints/Items/Ranged/F_Attach Structure"))
  (`parent.Set Static Attachment` `In Attachment`)
  (bind _asbp_character_template (cast `/Game/Blueprints/Core/BP_Character_Template` (`ActorComponent.GetOwner` (`.Component_16_7179BA4B403648FB10CC738584E38CE8` (break `/Game/Blueprints/Items/Ranged/F_Attach` `In Attachment`)))))
  (`self.Assign Ragdoll End` _asbp_character_template))

(event `self.Set Moving Attachment`
  (params (`In Character` :type "/Game/Blueprints/Core/BP_Character_Template Object Reference") (Hit :type "HitResult Structure (by ref)"))
  (`parent.Set Moving Attachment` `In Character` Hit)
  (`self.Assign Ragdoll End` `In Character`))

(event `Assign Ragdoll End`
  (params (InputPin :type "/Game/Blueprints/Core/BP_Character_Template Object Reference"))
  (add `/Game/Blueprints/Core/BP_Character_Template.OnRecovered` InputPin (delegate `OnRecovered_Event`))
  (add `/Game/Blueprints/Core/BP_Character_Template.OnRevived` InputPin (delegate `OnRecovered_Event`))
  (`KismetArrayLibrary.Array_Add` (`self.Ignore Characters`) InputPin))

(event `OnRecovered_Event`
  (params (Character :type "/Game/Blueprints/Core/BP_Character_Template Object Reference")))

(event `BP_Projectile_TripWire_AutoGenFunc`
  (params (OverlappedComponent :type "PrimitiveComponent Object Reference") (OtherActor :type "Actor Object Reference") (OtherComp :type "PrimitiveComponent Object Reference") (OtherBodyIndex :type Integer) (bFromSweep :type Boolean) (SweepResult :type "HitResult Structure (by ref)"))
  (`self.Trip Target` OtherActor SweepResult))

(fn `Can Trip`
  (params (Character :type "/Game/Blueprints/Core/BP_Character_Template Object Reference"))
  (returns (Can :type Boolean))
  (if (`KismetArrayLibrary.Array_Contains` (`self.Ignore Characters`) Character)
    (return false)
    (else
      (for _array_element (`self.Attached Wires`)
        (`/Engine/EditorBlueprintResources/StandardMacros.IsValid` _array_element
          (:`Is Valid`
            (if (`KismetArrayLibrary.Array_Contains` (`/Game/Blueprints/Items/Ranged/BP_Projectile_TripWire.Ignore Characters` _array_element) (`local.Character`))
              (return false)))))
      (return (not (`GSCBlueprintFunctionLibrary.HasMatchingGameplayTag` (`local.Character`) (`BlueprintGameplayTagLibrary.MakeLiteralGameplayTag` (struct :`TagName` "Status.Invulnerable"))))))))

(fn `Connect Tripwire`
  (bind _attached_wires (`self.Attached Wires`))
  (bind (_outactors _returnvalue) (`KismetSystemLibrary.SphereOverlapActors` (`self.K2_GetActorLocation`) (`self.Tripwire Range`) (`|MakeArray` "ObjectTypeQuery9" :!type "EObjectTypeQuery Enum") "BP_Projectile_TripWire_C" (`|MakeArray` self :!type "Actor Object Reference")))
  (if _returnvalue
    (for _array_element _outactors
      (bind _asbp_projectile_trip_wire (cast `/Game/Blueprints/Items/Ranged/BP_Projectile_TripWire` _array_element))
      (`KismetArrayLibrary.Array_Add` _attached_wires _asbp_projectile_trip_wire)
      (set `self.Attached Wires` _attached_wires) ; triggers onrep
    )))

(fn `Create Wire`
  (params (`Target Component` :type "SceneComponent Object Reference"))
  (bind _returnvalue (`AddComponent|NODE_AddTripWireComponent-0` :`bManualAttachment` true :`Target Component` `Target Component`))
  (`SceneComponent.K2_AttachToComponent` _returnvalue (`self.WireRoot`) "None" "SnapToTarget" "SnapToTarget" "KeepWorld" true)
  (add `PrimitiveComponent.OnComponentBeginOverlap` _returnvalue (`|CreateDelegate` :!event `BP_Projectile_TripWire_AutoGenFunc`)))

(fn `Deal Damage`
  (params (`Damaged Actor` :type "Actor Object Reference") (`Other Comp` :type "PrimitiveComponent Object Reference") (Hit :type "HitResult Structure (by ref)"))
  (locals (`L Bone` :type Name) (`L Attachment` :type "/Game/Blueprints/Items/Ranged/F_Attach Structure"))
  (`parent.Deal Damage` `Damaged Actor` `Other Comp` Hit)
  (`self.Connect Tripwire`)
  (return))

(fn `Destroy All Wires`
  (for _array_element (`SceneComponent.GetChildrenComponents` (`self.WireRoot`) false)
    (`/Engine/EditorBlueprintResources/StandardMacros.IsValid` _array_element
      (:`Is Valid`
        (`ActorComponent.K2_DestroyComponent` _array_element)))))

(fn `Get Always Show Widget`
  (returns (`Always Show` :type Boolean))
  (return false))

(fn `Get Interact Distance`
  (returns (Distance :type "Float (double-precision)"))
  (return 250.0))

(fn `Get Interact Duration`
  (returns (Duration :type "Float (double-precision)"))
  (return 0.0))

(fn `Get Interact Text`
  (returns (Text :type Text))
  (return "Pickup Bolt"))

(fn `Get Interact Widget Class`
  (returns (`Widget Class` :type "/Game/Primer/Primer_Interaction/UI/W_Interact_Master Soft Class Reference"))
  (return "/Game/Primer/Primer_Interaction/UI/W_Interact_Basic.W_Interact_Basic_C"))

(fn `OnAttachDestroyed`
  (params (DestroyedActor :type "Actor Object Reference"))
  ;[1 1 1] Tripwire doesn't die on attached destroy
  ; because snapshots destroy AI
  ; and then this tripwire would dissapear
)

(fn `OnAttachFractured`
  (params (Actor :type "/Game/Blueprints/Fracture/FractureCore/BP_FractureActor Object Reference"))
  (`self.K2_DestroyActor`))

(fn `OnRep_Attached Wires`
  (`self.Update Tripwire`))

(fn `Trip Target`
  (params (Object :type "Object Object Reference") (Hit :type "HitResult Structure (by ref)"))
  (locals (`L Velocity` :type "Vector Structure" :default (0.0 0.0 0.0)))
  (bind (_bblockinghit _binitialoverlap _time _distance _location) (`GameplayStatics.BreakHitResult` Hit))
  (bind _asbp_character_template (cast `/Game/Blueprints/Core/BP_Character_Template` Object))
  (if (`self.Can Trip` _asbp_character_template)
    (`GameplayStatics.PlaySoundAtLocation` "/Game/Blueprints/Items/Ranged/A_Twang_Cue.A_Twang_Cue" _location (struct) 1.0 1.0 0.0 null null null null)
    (`/Engine/EditorBlueprintResources/ActorMacros.Switch Has Authority`
      (:`Authority`
        (set `local.L Velocity` (`self.GetVelocity` _asbp_character_template))
        (`/Game/Blueprints/Core/BP_Character_Template.Enter KO` _asbp_character_template)
        (bind _mesh (`Character.Mesh` _asbp_character_template))
        (if (`SceneComponent.IsAnySimulatingPhysics` _mesh)
          (`PrimitiveComponent.AddImpulseAtLocation` _mesh (+ (* (`local.L Velocity`) 15.0) (0.0 0.0 7000.0)) _location (`.ReturnValue` (`SkinnedMeshComponent.FindClosestBone_K2` (`Character.Mesh` _asbp_character_template) _location 0.0 false))))))))

(fn `Update Tripwire`
  (`|ExecutionSequence`
    (:`then_0`
      (`/Engine/EditorBlueprintResources/StandardMacros.Can Execute Cosmetic Events`
        (:`True`
          (`self.Destroy All Wires`)
          (if (`KismetArrayLibrary.Array_IsNotEmpty` (`self.Attached Wires`))
            (for _array_element (`self.Attached Wires`)
              (`/Engine/EditorBlueprintResources/StandardMacros.IsValid` _array_element
                (:`Is Valid`
                  (`self.Create Wire` (`/Game/Blueprints/Items/Ranged/BP_Projectile_TripWire.WireRoot` _array_element)))))))))
    (:`then_1`
      (`/Engine/EditorBlueprintResources/ActorMacros.Switch Has Authority`
        (:`Authority`
          (bind (_arrayindex _arrayelement) (`/Engine/EditorBlueprintResources/StandardMacros.ReverseForEachLoop` (`self.Attached Wires`))
            (:`LoopBody`
              (`/Engine/EditorBlueprintResources/StandardMacros.IsValid` _arrayelement
                (:`Is Valid`
                  (if (> (`KismetMathLibrary.Vector_Distance` (`SceneComponent.K2_GetComponentLocation` (`/Game/Blueprints/Items/Ranged/BP_Projectile_TripWire.WireRoot` _arrayelement)) (`SceneComponent.K2_GetComponentLocation` (`self.WireRoot`))) (`self.Tripwire Range`))
                    (`KismetArrayLibrary.Array_RemoveItem` (`self.Attached Wires`) _arrayelement)))
                (:`Is Not Valid`
                  (`KismetArrayLibrary.Array_Remove` (`self.Attached Wires`) _arrayindex))))))))))

(fn `UserConstructionScript`
  (`parent.UserConstructionScript`))