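; Sling ranged weapon item that spins around its roll axis while its owner has the State.Aiming tag, and otherwise resets to its default rotation.
; Interacting first tries to consume it through BPItemAmmo, destroying it on success and otherwise running the parent interaction.
; When ammo hits zero, the server drops and destroys it.
; The muzzle transform derives from the owning character's eye viewpoint, offset forward and right.
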(event `self.ReceiveTick`
  (params (DeltaSeconds :type "Float (single-precision)"))
  (bind _returnvalue (`self.GetOwner`))
  (`/Engine/EditorBlueprintResources/StandardMacros.IsValid` _returnvalue
    (:`Is Valid`
      (if (`GSCBlueprintFunctionLibrary.HasMatchingGameplayTag` _returnvalue (struct :`TagName` "State.Aiming"))
        (`self.K2_AddActorLocalRotation` (`KismetMathLibrary.MakeRotator` (* (`self.Swing Speed`) DeltaSeconds -1.0)))
        (else
          (`self.K2_SetActorRelativeRotation` (`self.Default Rotation`)))))))

(event `/Game/Primer/Primer_Interaction/BPI_Interact.Execute Interact`
  (params (User :type "Controller Object Reference"))
  (bind _consumed (`/Game/Blueprints/Items/BP_ItemAmmo.Consume` (`self.BP_ItemAmmo`) User))
  (if _consumed
    (`self.K2_DestroyActor`)
    (else
      (`parent.Execute Interact` User))))

(fn `Fire Projectile`
  (`parent.Fire Projectile`))

(fn `Get Muzzle`
  (returns (`World Transform` :type "Transform Structure"))
  (bind _ascharacter (cast `Character` (`self.GetOwner`)))
  (bind (_outlocation _outrotation) (`self.GetActorEyesViewPoint` _ascharacter))
  (return (`KismetMathLibrary.MakeTransform` (+ _outlocation (* (`KismetMathLibrary.GetForwardVector` _outrotation) 100.0) (* (`KismetMathLibrary.GetRightVector` _outrotation) 10.0)) _outrotation)))

(fn `OnAmmoUpdated`
  (`parent.OnAmmoUpdated`)
  (`/Engine/EditorBlueprintResources/ActorMacros.Switch Has Authority`
    (:`Authority`
      (if (== (`/Game/Blueprints/Items/BP_ItemAmmo.Ammo` (`self.BP_ItemAmmo`)) 0)
        (`self.Drop`)
        (`self.K2_DestroyActor`)))))

(fn `UserConstructionScript`
  (`parent.UserConstructionScript`))