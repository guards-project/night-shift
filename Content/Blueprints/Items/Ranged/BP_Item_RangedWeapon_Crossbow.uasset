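; Crossbow ranged weapon item that shows its remaining ammo on the weapon model.
; On ammo updates it gathers the item mesh's child components tagged "ammo" and swaps their materials by index.
; Meshes at or beyond the current ammo count get a transparent material, while the rest get the bow's polygon material.
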(fn `Get Ammo Meshes`
  (returns (`Out Ammo Meshes` :type "Array of SceneComponent Object Reference"))
  (locals (`L Ammo Meshes` :type "Array of SceneComponent Object Reference"))
  (for _array_element (`SceneComponent.GetChildrenComponents` (`self.Item Mesh`) false)
    (if (`ActorComponent.ComponentHasTag` _array_element "ammo")
      (`KismetArrayLibrary.Array_Add` (`local.L Ammo Meshes`) _array_element)))
  (return (`local.L Ammo Meshes`)))

(fn `OnAmmoUpdated`
  (`parent.OnAmmoUpdated`)
  (bind _out_ammo_meshes (`self.Get Ammo Meshes`))
  (for (_array_element _array_index) _out_ammo_meshes
    (bind _asprimitive_component (cast `PrimitiveComponent` _array_element))
    (`PrimitiveComponent.SetMaterial` _asprimitive_component 0 (select `bool` (>= _array_index (`/Game/Blueprints/Items/BP_ItemAmmo.Ammo` (`self.BP_ItemAmmo`))) :`false` "/Game/_Guards/Art/Materials/PolygonMaster/M_Polygon_Inst_Bow.M_Polygon_Inst_Bow" :`true` "/Game/_Guards/Art/Materials/Transparent/M_TransparentBasic_Inst.M_TransparentBasic_Inst" :!type "MaterialInterface Object Reference"))))

(fn `UserConstructionScript`
  (`parent.UserConstructionScript`))