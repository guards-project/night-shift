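; Ranged weapon item that fires projectiles from its muzzle, with ammo and reload.
; The authority runs single or timer-driven automatic fire; emptying stops firing and auto-reloads for BP_Polygon_AI owners.
; It leads the AI user's target, otherwise follows the owner's view while tagged State.Aiming.
; AI shots use gravity-aware suggested velocities with target lead and play an animated star cue, and a path-prediction helper traces the arc.
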(event `self.ReceiveBeginPlay`
  (`parent.ReceiveBeginPlay`)
  (if (`self.Auto Fire`)
    (`KismetSystemLibrary.Delay` (`self.Auto Fire Delay`))
    (`self.Start Firing`)))

(event `self.ReceiveTick`
  (params (DeltaSeconds :type "Float (single-precision)"))
  (bind _returnvalue (`self.GetOwner`))
  (`parent.ReceiveTick` DeltaSeconds)
  (`self.AI User`
    (:`then`
      (bind _success (`self.Aim at AI Target`))
      (if (not _success)
        (`/Engine/EditorBlueprintResources/StandardMacros.IsValid` _returnvalue :!label _label
          (:`Is Valid`
            (if (`GSCBlueprintFunctionLibrary.HasMatchingGameplayTag` _returnvalue (struct :`TagName` "State.Aiming"))
              (`self.Aim with Actor Eyes`))))))
    (:`else`
      (goto _label))))

(event `self.On Equipped`
  (params (NewOwner :type "Actor Object Reference"))
  (bind _returnvalue (`AIBlueprintHelperLibrary.GetAIController` (`self.GetOwner`)))
  (`parent.On Equipped` NewOwner)
  (bind _last_owner (`self.Last Owner`)
    (:`then`
      (bind _asbp_character_template (cast `/Game/Blueprints/Core/BP_Character_Template` _last_owner))
      (add `/Game/Blueprints/Core/BP_Character_Template.OnDied` _asbp_character_template (delegate `OnDied_Event`))
      (`/Engine/EditorBlueprintResources/StandardMacros.IsValid` _returnvalue
        (:`Is Valid`
          (bind _asai_controller_polygon (cast `/Game/Blueprints/Core/PolygonAI/Behaviour/AI_Controller_Polygon` _returnvalue))
          (add `/Game/Blueprints/Core/PolygonAI/Behaviour/AI_Controller_Polygon.Target Changed` _asai_controller_polygon (delegate `Target Changed_Event`))
          (set `self.AI User` _asai_controller_polygon))))
    (:`else`)))

(event `Target Changed_Event`
  (params (Controller :type "/Game/Blueprints/Core/PolygonAI/Behaviour/AI_Controller_Polygon Object Reference"))
  (`/Engine/EditorBlueprintResources/StandardMacros.IsValid` (`/Game/Blueprints/Core/PolygonAI/Behaviour/AI_Controller_Polygon.Get Current Target` Controller)
    (:`Is Valid`
      (`AbilitySystemBlueprintLibrary.AddLooseGameplayTags` (`self.GetOwner`) (`BlueprintGameplayTagLibrary.MakeLiteralGameplayTagContainer` (struct :`GameplayTags` (struct :`(TagName` "State.Aiming")))) true))
    (:`Is Not Valid`
      (`self.Stop Firing`)
      (`AbilitySystemBlueprintLibrary.RemoveLooseGameplayTags` (`self.GetOwner`) (`BlueprintGameplayTagLibrary.MakeLiteralGameplayTagContainer` (struct :`GameplayTags` (struct :`(TagName` "State.Aiming")))) true))))

(event `OnDied_Event`
  (params (Character :type "/Game/Blueprints/Core/BP_Character_Template Object Reference"))
  (`self.Stop Firing`))

(event `self.On Unequipped`
  (`parent.On Unequipped`)
  (bind _ai_user (`self.AI User`)
    (:`then`
      (remove `/Game/Blueprints/Core/PolygonAI/Behaviour/AI_Controller_Polygon.Target Changed` _ai_user (`|CreateDelegate` :!event `Target Changed_Event`))
      (set `self.AI User` null)
      (`self.Stop Firing`)
      (bind _last_owner (`self.Last Owner`)
        (:`then`
          (bind _asbp_character_template (cast `/Game/Blueprints/Core/BP_Character_Template` _last_owner))
          (remove `/Game/Blueprints/Core/BP_Character_Template.OnDied` _asbp_character_template (`|CreateDelegate` :!event `OnDied_Event`)))
        (:`else`)))
    (:`else`)))

(event `Delayed Reaction`
  (`KismetSystemLibrary.Delay` (`KismetMathLibrary.RandomFloatInRange` 0.2 0.6))
  (`self.Fire Projectile`))

(event `MC Star Anim`
  (`/Engine/EditorBlueprintResources/StandardMacros.Can Execute Cosmetic Events`
    (:`True`
      (`TimelineComponent.SetPlayRate` (`self.Animate Aiming Star`) (/ 1.0 (`self.Fire Rate`)))
      (`SceneComponent.SetVisibility` (`self.Star`) true false)
      (bind (_direction _alpha) (`Timeline|Animate Aiming Star` :!via `PlayFromStart`)
        (:`Update`
          (`SceneComponent.SetWorldScale3D` (`self.Star`) (`KismetMathLibrary.Conv_DoubleToVector` (`KismetMathLibrary.Lerp` 0.5 3.0 _alpha)))
          (`SceneComponent.K2_SetRelativeRotation` (`self.StarRoot`) (`KismetMathLibrary.MakeRotator` (`KismetMathLibrary.Lerp` -50.0 0.0 _alpha)) false false))
        (:`Finished`
          (`SceneComponent.SetVisibility` (`self.Star`) false false))))))

(event `self.BP_ItemAmmo.Ammo Updated`
  (params (`Ammo Comp` :type "/Game/Blueprints/Items/BP_ItemAmmo Object Reference") (`New Ammo` :type Integer))
  (`self.OnAmmoUpdated`))

(event `Play Reload Anim`
  (bind _reload_montage (`self.Reload Montage`)
    (:`then`
      (bind _ascharacter (cast `Character` (`self.GetOwner`)))
      (`Character.PlayAnimMontage` _ascharacter _reload_montage 1.0 "None"))
    (:`else`)))

(fn `Aim at AI Target`
  (returns (Success :type Boolean))
  (bind _target (`/Game/Blueprints/Core/PolygonAI/Behaviour/AI_Controller_Polygon.Get Current Target` (`self.AI User`)))
  (bind _origin (`self.GetActorBounds` _target true false))
  (`/Engine/EditorBlueprintResources/StandardMacros.IsValid` (`/Game/Blueprints/Core/PolygonAI/Behaviour/AI_Controller_Polygon.Get Current Target` (`self.AI User`))
    (:`Is Valid`
      (`self.K2_SetActorRotation` (`KismetMathLibrary.FindLookAtRotation` (`self.K2_GetActorLocation`) (+ _origin (* (`self.GetVelocity` _target) (/ (`KismetMathLibrary.Vector_Distance` (`self.K2_GetActorLocation`) _origin) (`.Speed` (defaults `Object` (`self.Projectile Class`))))))))
      (`self.K2_AddActorLocalRotation` (struct :`Yaw` -90.0))
      (return true))
    (:`Is Not Valid`
      (return false))))

(fn `Aim with Actor Eyes`
  (bind _returnvalue (`self.GetOwner`))
  (`/Engine/EditorBlueprintResources/StandardMacros.IsValid` _returnvalue
    (:`Is Valid`
      (`self.K2_SetActorRotation` (`.OutRotation` (`self.GetActorEyesViewPoint` _returnvalue)))
      (`self.K2_AddActorLocalRotation` (struct :`Yaw` -90.0)))))

(fn `Can Auto Reload`
  (returns (bSuccess :type Boolean))
  (return (`.bSuccess` (cast `/Game/Blueprints/Core/PolygonAI/BP_Polygon_AI` (`self.GetOwner`) :!pure true))))

(fn `Can Fire`
  (returns (ReturnValue :type Boolean))
  (bind _bp_itemammo (`self.BP_ItemAmmo`)
    (:`then`
      (return (> (`/Game/Blueprints/Items/BP_ItemAmmo.Ammo` _bp_itemammo) 0)))
    (:`else`)))

(fn `Execute Reload`
  (bind _bp_itemammo (`self.BP_ItemAmmo`))
  (`/Engine/EditorBlueprintResources/ActorMacros.Switch Has Authority`
    (:`Authority`
      (set `/Game/Blueprints/Items/BP_ItemAmmo.Ammo` (`/Game/Blueprints/Items/BP_ItemAmmo.Max Ammo` _bp_itemammo) _bp_itemammo))))

(fn `Fire Projectile`
  (`/Engine/EditorBlueprintResources/ActorMacros.Switch Has Authority`
    (:`Authority`
      (bind _returnvalue (`|SpawnActorFromClass` (`self.Projectile Class`) (`self.Get Muzzle`) "AlwaysSpawn" "SelectDefaultAtRuntime" self (`self.Get Instigator`)))
      (`self.On Projectile Fired` _returnvalue)
      (bind _output_get (set `/Game/Blueprints/Items/BP_ItemAmmo.Ammo` (`KismetMathLibrary.Max` (- (`/Game/Blueprints/Items/BP_ItemAmmo.Ammo` (`self.BP_ItemAmmo`)) 1)) (`self.BP_ItemAmmo`)))
      (if (== _output_get 0)
        (`self.On Empty`)))))

(fn `Get Instigator`
  (returns (Instigator :type "Pawn Object Reference"))
  (bind _returnvalue (`self.GetOwner`))
  (`/Engine/EditorBlueprintResources/StandardMacros.IsValid` _returnvalue
    (:`Is Valid`
      (return (`Actor.Instigator` _returnvalue)))
    (:`Is Not Valid`
      (return null))))

(fn `Get Muzzle`
  (returns (`World Transform` :type "Transform Structure"))
  (return (`SceneComponent.GetSocketTransform` (`self.Item Mesh`) (`self.Muzzle Bone`) "RTS_World")))

(fn `Is Firing`
  (returns (ReturnValue :type Boolean))
  (return (`KismetSystemLibrary.K2_IsTimerActiveHandle` (`self.Shoot Timer`))))

(fn `On Empty`
  (`self.Stop Firing`)
  (if (`self.Can Auto Reload`)
    (`self.Start Reload`)))

(fn `On Projectile Fired`
  (params (Projectile :type "/Game/Blueprints/Items/Ranged/BP_Projectile Object Reference"))
  ;[1 1 1] Velocity set via BTService_CanAttack ranged prediction logic
  (`/Engine/EditorBlueprintResources/StandardMacros.IsValid` Projectile
    (:`Is Valid`
      (`self.AI User`
        (:`then`
          (bind _prediction_velocity (`self.Suggest Velocity` null))
          (set `MovementComponent.Velocity` _prediction_velocity (`/Game/Blueprints/Items/Ranged/BP_Projectile.ProjectileMovement` Projectile))
          (`self.MC Star Anim`))
        (:`else`)))))

(fn `OnAmmoUpdated`)

(fn `Predict Velocity`
  (params (`In Target` :type "Actor Object Reference"))
  (returns (OutHit :type "HitResult Structure") (OutPathPositions :type "Array of Vector Structure") (OutLastTraceDestination :type "Vector Structure") (ReturnValue :type Boolean) (`Predicted Velocity` :type "Vector Structure"))
  (locals (`L Muzzle Location` :type "Vector Structure") (`L Target Actor` :type "Actor Object Reference") (`L Prediction V` :type "Vector Structure"))
  (bind _world_transform_location (`KismetMathLibrary.BreakTransform` (`self.Get Muzzle`)))
  (bind _in_target (`local.In Target`))
  (`self.AI User`
    (:`then`
      (bind _ai_target (`self.AI Target`)
        (:`then`
          (set `local.L Target Actor` _ai_target))
        (:`else`)))
    (:`else`
      (`/Engine/EditorBlueprintResources/StandardMacros.IsValid` _in_target
        (:`Is Valid`
          (set `local.L Target Actor` _in_target)))))
  (bind _prediction_velocity (`self.Suggest Velocity` (`local.L Target Actor`)))
  (bind _output_get (set `local.L Prediction V` _prediction_velocity))
  (if (!= _output_get (0.0 0.0 0.0))
    (set `local.L Muzzle Location` _world_transform_location)
    (bind (_outhit _outpathpositions _outlasttracedestination _returnvalue) (`GameplayStatics.Blueprint_PredictProjectilePath_ByTraceChannel` (`local.L Muzzle Location`) (`local.L Prediction V`) true 10.0 "ECC_WorldStatic" false (`|MakeArray` self (`self.GetOwner`) :!type "Actor Object Reference") "None" 5.0 15.0 2.0 (* (`.Gravity Scale` (defaults `Object` (`self.Projectile Class`))) -980.0)))
    (return _outhit _outpathpositions _outlasttracedestination _returnvalue (`local.L Prediction V`))))

(fn `Start Firing`
  (bind _fire_rate (`self.Fire Rate`))
  (`/Engine/EditorBlueprintResources/ActorMacros.Switch Has Authority`
    (:`Authority`
      (if (not (`self.Is Firing`))
        (`self.Firing State Changed` true)
        (if (`self.Automatic`)
          (if (> _fire_rate 0.0)
            (bind _returnvalue (`KismetSystemLibrary.K2_SetTimerDelegate` (`|CreateDelegate` :!event `Fire Projectile`) _fire_rate true))
            (set `self.Shoot Timer` _returnvalue)
            (`self.AI User`
              (:`then`
                (`self.MC Star Anim`))
              (:`else`
                (`self.Fire Projectile`)))
            (else
              (`self.Fire Projectile` :!label _label)
              (`self.Stop Firing`)))
          (else
            (goto _label)))))))

(fn `Start Reload`
  (`|ExecutionSequence`
    (:`then_0`
      (`self.Play Reload Anim`))
    (:`then_1`
      (`KismetSystemLibrary.K2_SetTimerDelegate` (`|CreateDelegate` :!event `Execute Reload`) (`self.Reload Duration`)))))

(fn `Stop Firing`
  (`/Engine/EditorBlueprintResources/ActorMacros.Switch Has Authority`
    (:`Authority`
      (if (`self.Is Firing`)
        (`KismetSystemLibrary.K2_ClearAndInvalidateTimerHandle` (`self.Shoot Timer`))
        (`self.Firing State Changed` false)))))

(fn `Suggest Velocity`
  (params (`In Target` :type "Actor Object Reference") (`Z Offset` :type "Float (double-precision)" :default -20.0))
  (returns (`Prediction Velocity` :type "Vector Structure"))
  (locals (`L Muzzle Location` :type "Vector Structure") (`L Target Actor` :type "Actor Object Reference"))
  (bind _world_transform_location (`KismetMathLibrary.BreakTransform` (`self.Get Muzzle`)))
  (bind _in_target (`local.In Target`))
  (bind (_start_sound _speed _gravity_scale) (defaults `Object` (`self.Projectile Class`)))
  (bind _returnvalue (+ (`self.GetActorBounds` (`local.L Target Actor`) true false) (`KismetMathLibrary.MakeVector` 0.0 0.0 (`local.Z Offset`))))
  (`self.AI User`
    (:`then`
      (bind _ai_target (`self.AI Target`)
        (:`then`
          (set `local.L Target Actor` _ai_target))
        (:`else`)))
    (:`else`
      (`/Engine/EditorBlueprintResources/StandardMacros.IsValid` _in_target
        (:`Is Valid`
          (set `local.L Target Actor` _in_target)))))
  (set `local.L Muzzle Location` _world_transform_location)
  (bind (_tossvelocity _returnvalue_2) (`GameplayStatics.BlueprintSuggestProjectileVelocity` (`local.L Muzzle Location`) (+ _returnvalue (* (`self.GetVelocity` (`local.L Target Actor`)) (/ (`KismetMathLibrary.Vector_Distance` _world_transform_location _returnvalue) (`.Speed` (defaults `Object` (`self.Projectile Class`)))))) _speed (* _gravity_scale -980.0) "DoNotTrace" 10.0))
  (if _returnvalue_2
    (return _tossvelocity)
    (else
      (return (0.0 0.0 0.0)))))

(fn `UserConstructionScript`
  (`parent.UserConstructionScript`))