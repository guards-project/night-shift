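; Sling rock projectile that deals damage on a hit, then becomes an interactable pickup with an outline-ready custom depth focus.
; The server sets replicated CanPickup after damage, blocking further damage; its RepNotify swaps projectile movement for simulated physics with gravity.
; Interacting uses the parent rearm logic when possible; otherwise the server spawns a sling with one ammo and equips it to the user.
; Either path destroys the rock.
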(event `self.ReceiveDestroyed`
  (`parent.ReceiveDestroyed`))

(event `/Game/Primer/Primer_Interaction/BPI_Interact.Start Focus`
  (`PrimitiveComponent.SetRenderCustomDepth` (`self.StaticMesh`) true))

(event `/Game/Primer/Primer_Interaction/BPI_Interact.Stop Focus`
  (`PrimitiveComponent.SetRenderCustomDepth` (`self.StaticMesh`) false))

(event `/Game/Primer/Primer_Interaction/BPI_Interact.Execute Interact`
  (params (User :type "Controller Object Reference"))
  (bind _returnvalue (`self.Can Rearm`))
  (if _returnvalue
    (`parent.Execute Interact` User)
    (`self.K2_DestroyActor`)
    (else
      (`/Engine/EditorBlueprintResources/ActorMacros.Switch Has Authority`
        (:`Authority`
          (bind _returnvalue_2 (`|SpawnActorFromClass` "/Game/Blueprints/Items/Ranged/BP_Item_RangedWeapon_Sling.BP_Item_RangedWeapon_Sling_C" (`KismetMathLibrary.Conv_VectorToTransform` (0.0 0.0 0.0)) "Undefined" "MultiplyWithRoot" null false null))
          (set `/Game/Blueprints/Items/BP_ItemAmmo.Ammo` 1 (`/Game/Blueprints/Items/Ranged/BP_Item_RangedWeapon.BP_ItemAmmo` _returnvalue_2))
          (`/Game/Blueprints/Items/BP_Inventory_Component.Equip Item` (`self.GetComponentByClass` (`Controller.K2_GetPawn` User) "/Game/Blueprints/Items/BP_Inventory_Component.BP_Inventory_Component_C") _returnvalue_2)
          (`self.K2_DestroyActor`))))))

(fn `Deal Damage`
  (params (`Damaged Actor` :type "Actor Object Reference") (`Other Comp` :type "PrimitiveComponent Object Reference") (Hit :type "HitResult Structure (by ref)"))
  (if (`self.Can Pickup`)
    (return)
    (else
      (`parent.Deal Damage` `Damaged Actor` `Other Comp` Hit)
      (`/Engine/EditorBlueprintResources/ActorMacros.Switch Has Authority`
        (:`Authority`
          (set `self.Can Pickup` true))
        (:`Remote`
          _))
      (return))))

(fn `Get Always Show Widget`
  (returns (`Always Show` :type Boolean))
  (return false))

(fn `Get Can Interact`
  (returns (ReturnValue :type Boolean))
  (return true))

(fn `Get Interact Distance`
  (returns (Distance :type "Float (double-precision)"))
  (return 250.0))

(fn `Get Interact Duration`
  (returns (Duration :type "Float (double-precision)"))
  (return 0.0))

(fn `Get Interact Text`
  (returns (Text :type Text))
  (return "Pickup Sling Rock"))

(fn `Get Interact Widget Class`
  (returns (`Widget Class` :type "/Game/Primer/Primer_Interaction/UI/W_Interact_Master Soft Class Reference"))
  (return "/Game/Primer/Primer_Interaction/UI/W_Interact_Basic.W_Interact_Basic_C"))

(fn `OnRep_Can Pickup`
  (`self.Update Physics`))

(fn `Update Physics`
  (bind _sphere (`self.Sphere`))
  (if (`self.Can Pickup`)
    (`ActorComponent.SetActive` (`self.ProjectileMovement`) false false)
    (`PrimitiveComponent.SetSimulatePhysics` _sphere true)
    (`PrimitiveComponent.SetEnableGravity` _sphere true)
    (`self.Disable Overlaps`)
    (`ProjectileMovementComponent.SetInterpolatedComponent` (`self.ProjectileMovement`) (`self.StaticMesh`))))

(fn `UserConstructionScript`
  (`parent.UserConstructionScript`))