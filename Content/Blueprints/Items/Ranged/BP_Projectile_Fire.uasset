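; Fire variant of a ranged projectile that sets off a Molotov explosion where it hits.
; On hit, the server spawns a BP_Item_Molotov at the projectile's transform, fills its LastHit with that location and triggers it immediately, reusing the Molotov's explosion logic.
; The fire trail particle is then deactivated and the parent class's hit handling runs.
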(event `self.On Hit Event`
  (params (ThisComponent :type "PrimitiveComponent Object Reference") (OtherActor :type "Actor Object Reference") (OtherComp :type "PrimitiveComponent Object Reference") (Hit :type "HitResult Structure (by ref)"))
  (`|ExecutionSequence`
    (:`then_0`
      (`/Engine/EditorBlueprintResources/ActorMacros.Switch Has Authority`
        (:`Authority`
          (bind _returnvalue (`|SpawnActorFromClass` "/Game/Blueprints/Items/Grenades/BP_Item_Molotov.BP_Item_Molotov_C" (`self.GetTransform`) "AlwaysSpawn" "MultiplyWithRoot" null false null))
          (set `/Game/Blueprints/Items/BP_Item.Last Hit` (`GameplayStatics.MakeHitResult` false false 0.0 0.0 (`self.K2_GetActorLocation`)) _returnvalue)
          (`/Game/Blueprints/Items/Grenades/BP_Item_Grenade.Server Init Explode` _returnvalue))))
    (:`then_1`
      (`ActorComponent.Deactivate` (`self.P_Trail_Fire`))
      (`parent.On Hit Event` ThisComponent OtherActor OtherComp Hit))))

(fn `UserConstructionScript`
  (`parent.UserConstructionScript`))