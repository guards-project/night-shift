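; Networked constraint actor that pins a character ragdoll bone to a replicated anchor to keep its position in sync.
; The server moves the actor to the bone every tick, while clients build the physics constraint on BeginPlay.
; Constraint replication snaps the ragdoll onto the actor, offset by its pelvis, and rebinds the constraint.
; It clears the constraint on destruction and self-destroys when the ragdoll is invalid (server) or destroyed (client binding).
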(event `self.ReceiveBeginPlay`
  (bind (_component1 _bone1 _component2 _bone2) (break `/Game/Blueprints/Items/Ranged/F_Constraint` (`self.Constraint`)))
  (`/Engine/EditorBlueprintResources/ActorMacros.Switch Has Authority` ; override parent begin \nclients create a constraint\nserver only updates the location
    (:`Remote`
      (`PhysicsConstraintComponent.SetConstrainedComponents` (`self.PhysicsConstraint`) _component1 _bone1 (`self.Primitive`) _bone2)
      (add `self.OnEndPlay` (`ActorComponent.GetOwner` _component1) (delegate `OnEndPlay_Event`)))))

(event `OnEndPlay_Event` :!signature `self.OnEndPlay`
  (params (Actor :type "Actor Object Reference") (EndPlayReason :type "EEndPlayReason Enum" :default "Destroyed"))
  (switch `EEndPlayReason` EndPlayReason
    (:`Destroyed`
      (`self.K2_DestroyActor`) ; destroy self
    )))

(event `self.ReceiveTick`
  (params (DeltaSeconds :type "Float (single-precision)"))
  (bind (_component1 _bone1) (break `/Game/Blueprints/Items/Ranged/F_Constraint` (`self.Constraint`)))
  (`/Engine/EditorBlueprintResources/ActorMacros.Switch Has Authority` ; if we have an owner, then we are simulating the CharacterTemplate Ragdoll, only the server updates the location of the constraint
    (:`Authority`
      (`/Engine/EditorBlueprintResources/StandardMacros.IsValid` _component1
        (:`Is Valid`
          (`self.K2_SetActorTransform` (`KismetMathLibrary.MakeTransform` (.location (`SceneComponent.GetSocketTransform` _component1 _bone1 "RTS_World")) (.rotation (`SceneComponent.GetSocketTransform` _component1 _bone1 "RTS_World"))) false true))))))

(event `self.ReceiveDestroyed`
  (`PhysicsConstraintComponent.SetConstrainedComponents` (`self.PhysicsConstraint`) null "None" null "None"))

(fn `OnRep_Constraint`
  (`self.Update Constraint`))

(fn `Update Constraint`
  (bind (_component1 _bone1 _component2 _bone2) (break `/Game/Blueprints/Items/Ranged/F_Constraint` (`self.Constraint`)))
  (bind ((`Component1_10_7179BA4B403648FB10CC738584E38CE8` _component1_2)) (break `/Game/Blueprints/Items/Ranged/F_Constraint` (`self.Constraint`)))
  (bind _returnvalue_location (`KismetMathLibrary.BreakTransform` (`SceneComponent.GetSocketTransform` _component1_2 "Pelvis" "RTS_Component")))
  (`|ExecutionSequence`
    (:`then_0`
      (`/Engine/EditorBlueprintResources/StandardMacros.IsValid` (`.Component1_10_7179BA4B403648FB10CC738584E38CE8` (break `/Game/Blueprints/Items/Ranged/F_Constraint` (`self.Constraint`)))
        (:`Is Valid`
          (`SceneComponent.K2_SetWorldTransform` _component1_2 (`self.GetTransform`) false true)
          (`SceneComponent.K2_AddLocalOffset` _component1_2 (* _returnvalue_location -1) false true))
        (:`Is Not Valid`
          (`/Engine/EditorBlueprintResources/ActorMacros.Switch Has Authority`
            (:`Authority`
              (`self.K2_DestroyActor`)
              (return))))))
    (:`then_1`
      (`PhysicsConstraintComponent.SetConstrainedComponents` (`self.PhysicsConstraint`) _component1 _bone1 (`self.Primitive`) _bone2))))

(fn `UserConstructionScript`)