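; Thrown poison bottle that bursts on impact into a cloud that drugs players and stuns AI.
; On the first hit it hides, and the authority briefly enables an overlap sphere there to apply gameplay effects, once per player, then destroys the actor.
; Cosmetic-capable instances play the smash sound, explosion and short-lived volumetric cloud.
; While equipped, the mesh ignores physics bodies to avoid launching into the sky.
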(event `self.On Equipped`
  (params (NewOwner :type "Actor Object Reference"))
  ;[1 1 1] stops flying into sky
  (`parent.On Equipped` NewOwner)
  (`PrimitiveComponent.SetCollisionResponseToChannel` (`self.Item Mesh`) "ECC_PhysicsBody" "ECR_Ignore"))

(event `self.On Unequipped`
  ;[1 1 1] stops flying into sky
  (`parent.On Unequipped`)
  (`PrimitiveComponent.SetCollisionResponseToChannel` (`self.Item Mesh`) "ECC_PhysicsBody" "ECR_Block"))

(event `self.Execute Gameplay Thrown Hit Cue`
  (bind (_bblockinghit _binitialoverlap _time _distance _location) (`GameplayStatics.BreakHitResult` (`self.Last Hit`)))
  (`parent.Execute Gameplay Thrown Hit Cue`)
  (`/Engine/EditorBlueprintResources/StandardMacros.DoOnce` false
    (:`Completed`
      (`self.SetActorHiddenInGame` true)
      (`|ExecutionSequence`
        (:`then_0`
          (`/Engine/EditorBlueprintResources/ActorMacros.Switch Has Authority`
            (:`Authority`
              (`SceneComponent.K2_SetWorldLocation` (`self.Sphere`) (`.Location` (`GameplayStatics.BreakHitResult` (`self.Last Hit`))) false false)
              (`PrimitiveComponent.SetCollisionEnabled` (`self.Sphere`) "QueryOnly")
              (`KismetSystemLibrary.Delay` 0.5)
              (`PrimitiveComponent.SetCollisionEnabled` (`self.Sphere`) "NoCollision")
              (`KismetSystemLibrary.Delay` 1.0)
              (`self.K2_DestroyActor`))))
        (:`then_1`
          (`/Engine/EditorBlueprintResources/StandardMacros.Can Execute Cosmetic Events`
            (:`True`
              (`GameplayStatics.PlaySoundAtLocation` "/Game/_Guards/Audio/Hits/A_BottleSmash_Cue.A_BottleSmash_Cue" (`.Location` (`GameplayStatics.BreakHitResult` (`self.Last Hit`))) (struct) 1.0 1.0 0.0 null null null null)
              (`ActorComponent.Deactivate` (`self.Niagara`))
              (`ActorComponent.Deactivate` (`self.Niagara1`))
              (`NiagaraFunctionLibrary.SpawnSystemAtLocation` "/Game/TrailEffect/Fx/Niagara/NS_MiffExplosion.NS_MiffExplosion" _location)
              (bind _returnvalue (`|SpawnActorFromClass` "/Game/UltraVolumetrics/Blueprints/BP_UltraVolumetrics_Miff.BP_UltraVolumetrics_Miff_C" (`KismetMathLibrary.MakeTransform` _location) "Undefined" "MultiplyWithRoot" null "NewEnumerator0" 5.0 true 21.038341 -1.071999 3.277114 0.380952 (0.5 0.5 1.0) 2.0 1.0 (struct :`R` 0.739998 :`G` 0.499892 :`B` 1.0 :`A` 1.0) (struct :`R` 0.079448 :`G` 0.041378 :`B` 0.083333 :`A` 1.0) 0.0 0.0 -0.2 0.0 6000.0 1.612889 false 0.0 1.737688 0.180952 0.5 null))
              (`self.SetLifeSpan` _returnvalue 4.0))))))))

(event `self.Sphere.OnComponentBeginOverlap`
  (params (OverlappedComponent :type "PrimitiveComponent Object Reference") (OtherActor :type "Actor Object Reference") (OtherComp :type "PrimitiveComponent Object Reference") (OtherBodyIndex :type Integer) (bFromSweep :type Boolean) (SweepResult :type "HitResult Structure (by ref)"))
  (`|ExecutionSequence`
    (:`then_0`
      (bind _asbp_character_template_player (cast `/Game/Blueprints/Core/BP_Character_Template_Player` OtherActor))
      (if (not (`KismetArrayLibrary.Array_Contains` (`self.Drugged`) _asbp_character_template_player))
        (`KismetArrayLibrary.Array_AddUnique` (`self.Drugged`) _asbp_character_template_player)
        (bind _returnvalue (`AbilitySystemBlueprintLibrary.GetAbilitySystemComponent` _asbp_character_template_player))
        (`AbilitySystemComponent.BP_ApplyGameplayEffectToSelf` _returnvalue "/Game/Blueprints/Items/Interactable/Pickups/GE_DrugCloud_Weak.GE_DrugCloud_Weak_C" 6.0 (`AbilitySystemComponent.MakeEffectContext` _returnvalue))))
    (:`then_1`
      (bind _asbp_polygon_ai (cast `/Game/Blueprints/Core/PolygonAI/BP_Polygon_AI` OtherActor))
      (bind _returnvalue_2 (`AbilitySystemBlueprintLibrary.GetAbilitySystemComponent` _asbp_polygon_ai))
      (`AbilitySystemComponent.BP_ApplyGameplayEffectToSelf` _returnvalue_2 "/Game/Blueprints/GAS/Effects/GE_Stun.GE_Stun_C" 2.0 (`AbilitySystemComponent.MakeEffectContext` _returnvalue_2)))))

(fn `UserConstructionScript`
  (`parent.UserConstructionScript`))