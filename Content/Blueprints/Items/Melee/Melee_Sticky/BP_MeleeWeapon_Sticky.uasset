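; Throwable, stackable melee weapon (e.g. knife) that sticks into whatever it damages.
; Throwing adds spin and equips a spawned copy holding the remaining ammo; interacting merges ammo or falls back to normal pickup.
; On the server it attaches to the hit component or bone, aligning by cached pre-impact velocity for characters and traced surface normals otherwise.
; A replicated attachment transform syncs clients, and physics resumes if an unowned weapon's host is destroyed.
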(event `self.ReceiveTick`
  (params (DeltaSeconds :type "Float (single-precision)"))
  ;[1 1 1] Cache last velocity before hit (which is 0 velocity)
  ; So that we can use if for attachment math
  (`parent.ReceiveTick` DeltaSeconds)
  (set `self.Last V` (`self.GetVelocity`)))

(event `self.Apply Thrown Damage`
  ;[1 1 1] When thrown damage is applied, attach to 'last hit'
  (`parent.Apply Thrown Damage`)
  (`self.Attach`))

(event `self.Throw Item`
  (params (Location :type "Vector Structure") (Impulse :type "Vector Structure") (Torque :type "Vector Structure") (Thrown :type Boolean))
  ;[1 1 1] When this weapon is thrown, spin and set ammo to 1. Spawn equip another of this item with -1 ammo.
  (`parent.Throw Item` Location Impulse Torque Thrown)
  (`|ExecutionSequence`
    (:`then_0`
      (if (> (`self.Throw Torque`) 0.0)
        (`PrimitiveComponent.AddTorqueInDegrees` (`self.Item Mesh`) (* (`self.GetActorRightVector` (`self.Last Owner`)) (`self.Throw Torque`)) "None" true)))
    (:`then_1`
      (`/Engine/EditorBlueprintResources/ActorMacros.Switch Has Authority`
        (:`Authority`
          (`self.SetActorTickEnabled` true)
          (if (> (`/Game/Blueprints/Items/BP_ItemAmmo.Ammo` (`self.BP_ItemAmmo`)) 1)
            (bind _returnvalue (`|SpawnActorFromClass` (castclass `/Game/Blueprints/Items/Melee/Melee_Sticky/BP_MeleeWeapon_Sticky` (`GameplayStatics.GetObjectClass` self) :!pure true) (`KismetMathLibrary.Conv_VectorToTransform` (0.0 0.0 0.0)) "AlwaysSpawn" "MultiplyWithRoot" null (`self.Intigator Item`) false null))
            (set `/Game/Blueprints/Items/BP_ItemAmmo.Ammo` (- (`/Game/Blueprints/Items/BP_ItemAmmo.Ammo` (`self.BP_ItemAmmo`)) 1) (`/Game/Blueprints/Items/Melee/Melee_Sticky/BP_MeleeWeapon_Sticky.BP_ItemAmmo` _returnvalue))
            (`/Game/Blueprints/Items/BP_Inventory_Component.Equip Item` (`self.GetComponentByClass` (`self.Last Owner`) "/Game/Blueprints/Items/BP_Inventory_Component.BP_Inventory_Component_C") _returnvalue)
            (set `/Game/Blueprints/Items/BP_ItemAmmo.Ammo` 1 (`self.BP_ItemAmmo`))
            (`self.New Item Created` self _returnvalue)))))))

(event `/Game/Primer/Primer_Interaction/BPI_Interact.Execute Interact`
  (params (User :type "Controller Object Reference"))
  ;[1 1 1] When Interacting with this weapon
  ; If its a knife, Add 1 ammo to the held item, don't pickup and destroy the knife instead
  ; Otherwise, if its a different weapon, continue the normal flow (drop held item, and pickup other item)
  (`/Engine/EditorBlueprintResources/ActorMacros.Switch Has Authority`
    (:`Authority`
      (bind _consumed (`/Game/Blueprints/Items/BP_ItemAmmo.Consume` (`self.BP_ItemAmmo`) User))
      (if _consumed
        (if (== (`/Game/Blueprints/Items/BP_ItemAmmo.Ammo` (`self.BP_ItemAmmo`)) 0)
          (`self.K2_DestroyActor`))
        (else
          (`parent.Execute Interact` User) ; regular pickup
        )))))

(event `self.ReceiveEndPlay`
  (params (EndPlayReason :type "EEndPlayReason Enum" :default "Destroyed"))
  ;[1 1 1] On Destroy, assume we are picked up and play a sound
  (switch `EEndPlayReason` EndPlayReason
    (:`Destroyed`
      (`/Engine/EditorBlueprintResources/StandardMacros.Can Execute Cosmetic Events`
        (:`True`
          (`GameplayStatics.PlaySoundAtLocation` (`self.Pickup Sound`) (`self.K2_GetActorLocation`) (struct) 1.0 1.0 0.0 null null null null))))))

(fn `Attach`
  (bind _returnvalue (`self.K2_GetActorLocation`))
  (bind (_bblockinghit _binitialoverlap _time _distance _location _impactpoint _normal _impactnormal _physmat _hitactor _hitcomponent _hitbonename) (`GameplayStatics.BreakHitResult` (`self.Last Hit`)))
  (bind (_ascharacter _bsuccess) (cast `Character` _hitactor :!pure true))
  (bind _returnvalue_2 (* (`KismetMathLibrary.Normal` (`self.Last V`)) 1.0))
  (bind _returnvalue_3 (+ _returnvalue (* _returnvalue_2 150.0)))
  (bind _returnvalue_4 (+ _returnvalue (* _returnvalue_2 -10.0)))
  (`/Engine/EditorBlueprintResources/StandardMacros.IsValid` (`self.GetAttachParentActor`)
    (:`Is Not Valid`
      (`/Engine/EditorBlueprintResources/ActorMacros.Switch Has Authority`
        (:`Authority`
          (`self.SetActorTickEnabled` false)
          (cast `/Game/Blueprints/Fracture/FractureCore/BP_FractureActor` _hitactor
            (:`CastFailed`
              (set `self.Physics Enabled` false)
              (add `self.OnDestroyed` _hitactor (`|CreateDelegate` :!event `On Attchment Destroyed`))
              (`self.K2_AttachToComponent` _hitcomponent (select `bool` (== _hitbonename "None") :`false` _hitbonename :`true` (`self.Get Closest Bone Name` _hitactor)) (select `bool` _bsuccess :`false` "KeepWorld" :`true` "SnapToTarget" :!type "EAttachmentRule Enum") "KeepWorld" "KeepWorld" false)
              (if _bsuccess
                (`self.Update Rotation` (* (`KismetMathLibrary.Normal` (`self.Last V`)) 1.0) 4.0)
                (else
                  (bind (_outhit _returnvalue_5) (`KismetSystemLibrary.LineTraceSingle` :`Start` _returnvalue_4 :`End` _returnvalue_3 :`TraceChannel` "TraceTypeQuery1" :`bTraceComplex` true :`DrawDebugType` (`self.Draw Debug Type`))) ; if other
                  (if _returnvalue_5
                    (bind (_bblockinghit_2 _binitialoverlap_2 _time_2 _distance_2 _location_2 _impactpoint_2 _normal_2 _impactnormal_2) (`GameplayStatics.BreakHitResult` _outhit))
                    (`self.K2_SetActorLocation` _impactpoint_2)
                    (`self.Update Rotation` (* _impactnormal_2 -1.0))
                    (else
                      (bind (_outhit_2 _returnvalue_6) (`KismetSystemLibrary.SphereTraceSingle` :`Start` _returnvalue_4 :`End` _returnvalue_3 :`Radius` 30.0 :`TraceChannel` "TraceTypeQuery1" :`bTraceComplex` true :`DrawDebugType` (`self.Draw Debug Type`)))
                      (if _returnvalue_6
                        (bind (_bblockinghit_3 _binitialoverlap_3 _time_3 _distance_3 _location_3 _impactpoint_3 _normal_3 _impactnormal_3) (`GameplayStatics.BreakHitResult` _outhit_2))
                        (`self.K2_SetActorLocation` _impactpoint_3)
                        (`self.Update Rotation` (* _impactnormal_3 -1.0))))))))))))))

(fn `Get Closest Bone Name`
  (params (`In Actor` :type "Actor Object Reference"))
  (returns (ReturnValue :type Name))
  (bind _ascharacter (cast `Character` `In Actor`)
    (:`then`
      (return (`.ReturnValue` (`SkinnedMeshComponent.FindClosestBone_K2` (`Character.Mesh` _ascharacter) (`self.K2_GetActorLocation`) 0.0 true))))
    (:`CastFailed`
      (return "None"))))

(fn `Get Random Yaw`
  (returns (ReturnValue :type "Float (double-precision)"))
  (return (`KismetMathLibrary.RandomFloatInRange` 0.0 360.0)))

(fn `On Attchment Destroyed`
  (params (DestroyedActor :type "Actor Object Reference"))
  (`/Engine/EditorBlueprintResources/StandardMacros.IsValid` (`self.GetOwner`)
    (:`Is Not Valid`
      (set `self.Physics Enabled` true)
      (`self.SetActorTickEnabled` true))))

(fn `OnRep_Attachment`
  (bind (_component _bone) (break `/Game/Blueprints/Items/Ranged/F_Attach` (`self.Attachment`)))
  ;[1 1 1] Attach after disabling
  (`self.K2_AttachToComponent` _component _bone "SnapToTarget" "KeepWorld" "KeepWorld")
  (`self.K2_SetActorRelativeTransform` (`.RelativeTransform_14_37C4901A431BB85EFDCCE6A82E8ACA4E` (break `/Game/Blueprints/Items/Ranged/F_Attach` (`self.Attachment`)))))

(fn `Set Attachment`
  (params (Component :type "PrimitiveComponent Object Reference") (Bone :type Name))
  (`/Engine/EditorBlueprintResources/ActorMacros.Switch Has Authority`
    (:`Authority`
      (set `self.Attachment` (make `/Game/Blueprints/Items/Ranged/F_Attach` Component Bone (`KismetMathLibrary.MakeRelativeTransform` (`self.GetTransform`) (`SceneComponent.GetSocketTransform` Component Bone "RTS_World")))))))

(fn `Update Rotation`
  (params (Direction :type "Vector Structure (by ref)") (`Rot Jitter` :type "Float (double-precision)" :default 15.0))
  (bind _returnvalue (* `Rot Jitter` -1.0))
  (bind (_bblockinghit _binitialoverlap _time _distance _location _impactpoint _normal _impactnormal _physmat _hitactor _hitcomponent _hitbonename) (`GameplayStatics.BreakHitResult` (`self.Last Hit`)))
  (`self.K2_SetActorRotation` (`KismetMathLibrary.MakeRotFromZ` Direction))
  (`self.K2_AddActorLocalRotation` (`KismetMathLibrary.MakeRotator` (`KismetMathLibrary.RandomFloatInRange` _returnvalue `Rot Jitter`) (`KismetMathLibrary.RandomFloatInRange` _returnvalue `Rot Jitter`) (`self.Get Random Yaw`)))
  (`self.K2_SetActorLocation` (+ (`self.K2_GetActorLocation`) (* (`self.GetActorUpVector`) (`self.Inset`))))
  (`self.Set Attachment` _hitcomponent (select `bool` (== _hitbonename "None") :`false` _hitbonename :`true` (`self.Get Closest Bone Name` _hitactor))))

(fn `UserConstructionScript`
  (`parent.UserConstructionScript`))