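; Snowball throwable in the sticky melee weapon family that destroys itself on Attach instead of sticking.
; Thrown hits add a snowball GameplayCue on the hit actor, or the last owner if that actor has no ability system.
; MCPop cleans up snowballs when snow stops: it drops and disables collision, pops with particles and sound after a random cosmetic delay, and authority destroys it a second later.
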(event `MC Pop`
  (bind _returnvalue (`self.K2_GetActorLocation`))
  ;[1 1 1] Cleanup snowballs if snow stops
  (`self.Drop`)
  (`self.SetActorEnableCollision` false)
  (`|ExecutionSequence`
    (:`then_0`
      (`/Engine/EditorBlueprintResources/StandardMacros.Can Execute Cosmetic Events`
        (:`True`
          (`KismetSystemLibrary.Delay` (`KismetMathLibrary.RandomFloatInRange` 0.02 0.3))
          (`self.SetActorHiddenInGame` true)
          (`NiagaraFunctionLibrary.SpawnSystemAtLocation` "/Game/Shooter_VFXPack/Particles/Projectiles/P_Snowball.P_Snowball" _returnvalue)
          (`GameplayStatics.PlaySoundAtLocation` "/Game/Fantasy_Interface_SFX/cue/WeaponPickupSoft_Cue.WeaponPickupSoft_Cue" _returnvalue (struct) 1.0 1.0 0.0 null null null null))))
    (:`then_1`
      (`/Engine/EditorBlueprintResources/ActorMacros.Switch Has Authority`
        (:`Authority`
          (`KismetSystemLibrary.Delay` 1.0)
          (`self.K2_DestroyActor`))))))

(fn `Attach`
  (`self.K2_DestroyActor`))

(fn `Execute Gameplay Thrown Hit Cue`
  (bind (_bblockinghit _binitialoverlap _time _distance _location _impactpoint _normal _impactnormal _physmat _hitactor) (`GameplayStatics.BreakHitResult` (`self.Last Hit`)))
  (`parent.Execute Gameplay Thrown Hit Cue`)
  (`GameplayCueFunctionLibrary.ExecuteGameplayCueOnActor` (select `bool` (`KismetSystemLibrary.IsValid` (`AbilitySystemBlueprintLibrary.GetAbilitySystemComponent` _hitactor)) :`false` (`self.Last Owner`) :`true` _hitactor) (struct :`TagName` "GameplayCue.Hit.Snowball") (`self.Create Hit Params` _hitactor)))

(fn `UserConstructionScript`
  (`parent.UserConstructionScript`))