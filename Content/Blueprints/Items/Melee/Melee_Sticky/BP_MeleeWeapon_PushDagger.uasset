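; Push dagger melee weapon Blueprint that adds a second dagger in the wielder's left hand and customizes how it sticks into what it hits.
; On equip, the authority spawns the left-hand attachment on the character mesh's socket and cleans it up on unequip.
; Its UpdateRotation override replaces the parent's, orienting along the hit direction with random jitter, insetting it, then attaching to the hit bone or closest bone.
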(event `self.On Equipped`
  (params (NewOwner :type "Actor Object Reference"))
  (`parent.On Equipped` NewOwner)
  (`/Engine/EditorBlueprintResources/ActorMacros.Switch Has Authority`
    (:`Authority`
      (`/Engine/EditorBlueprintResources/StandardMacros.IsValid` NewOwner
        (:`Is Valid`
          (bind _ascharacter (cast `Character` NewOwner))
          (bind _returnvalue (`|SpawnActorFromClass` "/Game/Blueprints/Items/Melee/Melee_Sticky/BP_Attachment_PushDaggerLeft.BP_Attachment_PushDaggerLeft_C" (`KismetMathLibrary.Conv_VectorToTransform` (0.0 0.0 0.0)) "AlwaysSpawn" "MultiplyWithRoot" self (`Character.Mesh` _ascharacter) "LeftHand" null))
          (set `self.Hand 2 Dagger` _returnvalue))))))

(event `self.On Unequipped`
  (`parent.On Unequipped`)
  (bind _hand_2_dagger (`self.Hand 2 Dagger`)
    (:`then`
      (`/Game/Blueprints/Items/Attachments/BP_Attachment.Cleanup Attachment` _hand_2_dagger))
    (:`else`)))

(fn `Update Rotation`
  (params (Direction :type "Vector Structure (by ref)") (`Rot Jitter` :type "Float (double-precision)"))
  (bind _returnvalue (* `Rot Jitter` -1.0))
  (bind (_bblockinghit _binitialoverlap _time _distance _location _impactpoint _normal _impactnormal _physmat _hitactor _hitcomponent _hitbonename) (`GameplayStatics.BreakHitResult` (`self.Last Hit`)))
  (`self.K2_SetActorRotation` (`KismetMathLibrary.MakeRotFromY` Direction))
  (`self.K2_AddActorLocalRotation` (`KismetMathLibrary.MakeRotator` (`KismetMathLibrary.RandomFloatInRange` _returnvalue `Rot Jitter`) (`self.Get Random Yaw`) (`KismetMathLibrary.RandomFloatInRange` _returnvalue `Rot Jitter`)))
  (`self.K2_SetActorLocation` (+ (`self.K2_GetActorLocation`) (* (`self.GetActorRightVector`) (`self.Inset`))))
  (`self.Set Attachment` _hitcomponent (select `bool` (== _hitbonename "None") :`false` _hitbonename :`true` (`self.Get Closest Bone Name` _hitactor)))
  (return))

(fn `UserConstructionScript`
  (`parent.UserConstructionScript`))