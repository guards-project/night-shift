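; Exploder torch melee weapon that puts a second torch in the character's left hand and deals area damage when thrown.
; On equip, the server spawns the left-hand torch attachment on the mesh's hand socket, and unequip cleans it up.
; Thrown damage applies radial damage at the last hit location using an insta-kill damage type, with the weapon as damage causer.
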(event `self.On Equipped`
  (params (NewOwner :type "Actor Object Reference"))
  (`parent.On Equipped` NewOwner)
  (`/Engine/EditorBlueprintResources/ActorMacros.Switch Has Authority`
    (:`Authority`
      (`/Engine/EditorBlueprintResources/StandardMacros.IsValid` NewOwner
        (:`Is Valid`
          (bind _ascharacter (cast `Character` NewOwner))
          (bind _returnvalue (`|SpawnActorFromClass` "/Game/Blueprints/Items/Melee/Melee_Light/BP_Attachment_ExploderTorch_Left.BP_Attachment_ExploderTorch_Left_C" (`KismetMathLibrary.Conv_VectorToTransform` (0.0 0.0 0.0)) "AlwaysSpawn" "MultiplyWithRoot" self (`Character.Mesh` _ascharacter) "LeftHand" null))
          (set `self.Hand 2 Torch` _returnvalue))))))

(event `self.On Unequipped`
  (`parent.On Unequipped`)
  (bind _hand_2_torch (`self.Hand 2 Torch`)
    (:`then`
      (`/Game/Blueprints/Items/Attachments/BP_Attachment.Cleanup Attachment` _hand_2_torch))
    (:`else`)))

(event `self.Apply Thrown Damage`
  (`GameplayStatics.ApplyRadialDamage` :`BaseDamage` 50.0 :`Origin` (`.Location` (`GameplayStatics.BreakHitResult` (`self.Last Hit`))) :`DamageRadius` 500.0 :`DamageTypeClass` "/Game/Blueprints/Items/DamageTypes/DamageType_Polygon_Lethal_InstaKill.DamageType_Polygon_Lethal_InstaKill_C" :`DamageCauser` self :`InstigatedByController` null))

(fn `UserConstructionScript`
  (`parent.UserConstructionScript`))