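; Knuckle duster melee weapon that places a second duster on the wielder's left hand while equipped.
; On equip it hides its second item mesh and, on authority only, spawns a separate attachment actor on the character mesh's LeftHand socket.
; On unequip it shows the second mesh again and tells the spawned attachment to clean itself up.
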(event `/Game/Blueprints/Items/BP_Item.On Equipped`
  (params (NewOwner :type "Actor Object Reference"))
  (`parent.On Equipped` NewOwner)
  (`SceneComponent.SetVisibility` (`self.ItemMesh2`) false false)
  (`/Engine/EditorBlueprintResources/ActorMacros.Switch Has Authority`
    (:`Authority`
      (`/Engine/EditorBlueprintResources/StandardMacros.IsValid` NewOwner
        (:`Is Valid`
          (bind _ascharacter (cast `Character` NewOwner))
          (bind _returnvalue (`|SpawnActorFromClass` "/Game/Blueprints/Items/Melee/Melee_Light/BP_Attachment_KnuckleDust.BP_Attachment_KnuckleDust_C" (`KismetMathLibrary.Conv_VectorToTransform` (0.0 0.0 0.0)) "AlwaysSpawn" "MultiplyWithRoot" self (`Character.Mesh` _ascharacter) "LeftHand" null))
          (set `self.Hand 2 Knuckles` _returnvalue))))))

(event `/Game/Blueprints/Items/BP_Item.On Unequipped`
  (`parent.On Unequipped`)
  (`SceneComponent.SetVisibility` (`self.ItemMesh2`) true false)
  (bind _hand_2_knuckles (`self.Hand 2 Knuckles`)
    (:`then`
      (`/Game/Blueprints/Items/Attachments/BP_Attachment.Cleanup Attachment` _hand_2_knuckles))
    (:`else`)))

(fn `UserConstructionScript`
  (`parent.UserConstructionScript`))