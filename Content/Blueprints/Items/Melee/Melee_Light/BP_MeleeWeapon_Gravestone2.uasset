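; A gravestone melee weapon item that immobilizes an AI character equipping it and disables its own interaction.
; It binds to that character's state events, shrinking while the holder is knocked out or dead, restoring size on recovery or revive, and dropping when arrest state updates.
; The authority destroys it after thrown damage is applied, and destruction plays a smoke pop and stone-breaking sound.
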(event `self.On Equipped`
  (params (NewOwner :type "Actor Object Reference"))
  (`parent.On Equipped` NewOwner)
  (bind _asbp_polygon_ai (cast `/Game/Blueprints/Core/PolygonAI/BP_Polygon_AI` NewOwner))
  (`/Game/Blueprints/Core/BP_Character_Template.Auth Set Can Move` _asbp_polygon_ai false)
  (set `self.Can Ever Interact` false)
  (add `/Game/Blueprints/Core/BP_Character_Template.OnKO` _asbp_polygon_ai (delegate `On Downed`))
  (add `/Game/Blueprints/Core/BP_Character_Template.OnDied` _asbp_polygon_ai (delegate `On Downed`))
  (add `/Game/Blueprints/Core/BP_Character_Template.OnRecovered` _asbp_polygon_ai (delegate `On Recovered`))
  (add `/Game/Blueprints/Core/BP_Character_Template.OnRevived` _asbp_polygon_ai (delegate `On Recovered`))
  (add `/Game/Blueprints/Core/PolygonAI/BP_Polygon_AI.On Arrested Updated` _asbp_polygon_ai (delegate `On Arrested Updated_Event`)))

(event `On Downed`
  (params (Character :type "/Game/Blueprints/Core/BP_Character_Template Object Reference"))
  (`self.SetActorScale3D` (0.2 0.2 0.2)))

(event `On Recovered`
  (params (Character :type "/Game/Blueprints/Core/BP_Character_Template Object Reference"))
  (`self.SetActorScale3D` (1.0 1.0 1.0)))

(event `On Arrested Updated_Event`
  (params (Character :type "/Game/Blueprints/Core/BP_Character_Template Object Reference") (Arrested :type Boolean))
  (`self.Drop`))

(event `self.ReceiveEndPlay`
  (params (EndPlayReason :type "EEndPlayReason Enum" :default "Destroyed"))
  (bind _returnvalue (`self.K2_GetActorLocation`))
  (`parent.ReceiveEndPlay` EndPlayReason)
  (switch `EEndPlayReason` EndPlayReason
    (:`Destroyed`
      (`NiagaraFunctionLibrary.SpawnSystemAtLocation` "/Game/Shooter_VFXPack/Particles/HitsAndExplosions/NS_SmokePop.NS_SmokePop" _returnvalue)
      (`GameplayStatics.PlaySoundAtLocation` "/Game/Blueprints/GAS/Cues/Sounds/A_Break_Stone.A_Break_Stone" _returnvalue (struct) 1.0 1.0 0.0 "/Game/Blueprints/GAS/Cues/Sounds/ATT_Close.ATT_Close" null null null))))

(event `self.Apply Thrown Damage`
  (`parent.Apply Thrown Damage`)
  (`/Engine/EditorBlueprintResources/ActorMacros.Switch Has Authority`
    (:`Authority`
      (`self.K2_DestroyActor`))))

(fn `UserConstructionScript`
  (`parent.UserConstructionScript`))