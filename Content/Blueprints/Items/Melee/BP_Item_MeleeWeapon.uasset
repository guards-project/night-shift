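; Melee weapon item Blueprint that manages a Niagara trail effect on the weapon mesh.
; ActivateTrail waits for a delay, spawns the trail as a pooled attached system with a configurable offset, width and lifetime, then auto-deactivates it after a positive duration.
; The trail also deactivates when the weapon registers a hit or is destroyed, alongside the parent class behavior.
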(event `Activate Trail`
  (params (Delay :type "Float (single-precision)") (Duration :type "Float (single-precision)"))
  (`KismetSystemLibrary.Delay` Delay)
  (bind _returnvalue (`NiagaraFunctionLibrary.SpawnSystemAttached` (`self.Trail Effect`) (`self.Item Mesh`) "None" (0.0 0.0 0.0) (struct) "SnapToTarget" true true "AutoRelease"))
  (`SceneComponent.K2_SetRelativeTransform` _returnvalue (`self.Trail Offset`) false false)
  (set `self.NS_Trail` _returnvalue)
  (bind _ns_trail (`self.NS_Trail`)
    (:`then`
      (`NiagaraComponent.SetVariableFloat` _ns_trail "EffectWidthScale" (`self.Trail Width`))
      (`NiagaraComponent.SetVariableFloat` _ns_trail "LifeTime" (`self.Trail Life Time`))
      (if (> Duration 0.0)
        (`KismetSystemLibrary.Delay` Duration)
        (`self.Deactivate Trail`)))
    (:`else`)))

(event `Deactivate Trail`
  (bind _ns_trail (`self.NS_Trail`)
    (:`then`
      (`ActorComponent.Deactivate` _ns_trail))
    (:`else`)))

(event `self.ReceiveHit`
  (params (MyComp :type "PrimitiveComponent Object Reference") (Other :type "Actor Object Reference") (OtherComp :type "PrimitiveComponent Object Reference") (bSelfMoved :type Boolean) (HitLocation :type "Vector Structure") (HitNormal :type "Vector Structure") (NormalImpulse :type "Vector Structure") (Hit :type "HitResult Structure (by ref)"))
  (`parent.ReceiveHit` MyComp Other OtherComp bSelfMoved HitLocation HitNormal NormalImpulse Hit)
  (`self.Deactivate Trail`))

(event `self.ReceiveDestroyed`
  (`parent.ReceiveDestroyed`)
  (bind _ns_trail (`self.NS_Trail`)
    (:`then`
      (`ActorComponent.Deactivate` _ns_trail))
    (:`else`)))

(fn `UserConstructionScript`
  (`parent.UserConstructionScript`))