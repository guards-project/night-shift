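; Heavy melee scythe weapon that, when thrown, becomes a spinning, ricocheting projectile that kills characters it passes through.
; ThrowItem caches the thrower's view yaw, then Tick sweeps it along that direction without physics, reflecting horizontally on authority-side hits.
; While spinning, MurderSphere overlaps apply server-side insta-kill damage to characters except the last owner, plus death impulse and gore effects.
; Spinning ends after a timer, pickup or equip, restoring physics if unowned.
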(event `self.On Equipped`
  (params (NewOwner :type "Actor Object Reference"))
  (`parent.On Equipped` NewOwner)
  (`self.Stop Spinning`))

(event `self.Throw Item`
  (params (Location :type "Vector Structure") (Impulse :type "Vector Structure") (Torque :type "Vector Structure") (Thrown :type Boolean))
  (set `self.Thrown` Thrown)
  (`self.Cache Last Forward`)
  (`self.K2_SetActorLocation` (+ Location (* (`self.Last Forward`) 100.0) (0.0 0.0 -25.0)) false true)
  (`self.Start Spinning`)
  (`PrimitiveComponent.SetSimulatePhysics` (`self.Item Mesh`) false)
  (`/Engine/EditorBlueprintResources/ActorMacros.Switch Has Authority`
    (:`Authority`
      (set `self.Physics Enabled` false))))

(event `self.Pickup`
  (params (Controller :type "Controller Object Reference"))
  (`parent.Pickup` Controller)
  (`self.Stop Spinning`))

(event `Start Spinning`
  (bind _item_mesh (`self.Item Mesh`))
  (`self.Drop`)
  (`PrimitiveComponent.SetCollisionEnabled` (`self.Item Mesh`) "QueryAndPhysics")
  (`self.K2_SetActorRotation` (struct :`Roll` 90.0))
  (`PrimitiveComponent.SetCollisionEnabled` (`self.MurderSphere`) "QueryOnly")
  (`self.Activate Trail` 0.2 5.0)
  (`ActorComponent.Activate` (`self.RotatingMovement`) false)
  (`self.SetActorTickEnabled` true) ; enabled ricochet spinning
  (`PrimitiveComponent.SetCollisionEnabled` (`self.Item Mesh`) "QueryAndPhysics")
  (`PrimitiveComponent.SetCollisionResponseToAllChannels` _item_mesh "ECR_Ignore")
  (`PrimitiveComponent.SetCollisionResponseToChannel` _item_mesh "ECC_WorldDynamic" "ECR_Block")
  (`PrimitiveComponent.SetCollisionResponseToChannel` _item_mesh "ECC_WorldStatic" "ECR_Block")
  (`AudioComponent.Play` (`self.AudioSpin`) 0.0)
  (`KismetSystemLibrary.Delay` (`self.Spin Duration`))
  (`self.Stop Spinning`))

(event `Stop Spinning`
  (if (`self.IsActorTickEnabled`)
    (`|ExecutionSequence`
      (:`then_0`
        (`ActorComponent.Deactivate` (`self.RotatingMovement`))
        (bind _ns_trail (`self.NS_Trail`)
          (:`then`
            (`ActorComponent.Deactivate` _ns_trail))
          (:`else`)))
      (:`then_1`
        (`self.SetActorTickEnabled` false) ; disable ricochet spinning
        (`PrimitiveComponent.SetCollisionResponseToChannel` (`self.Item Mesh`) "ECC_Pawn" "ECR_Block")
        (`AudioComponent.Stop` (`self.AudioSpin`))
        (`/Engine/EditorBlueprintResources/ActorMacros.Switch Has Authority`
          (:`Authority`
            (`/Engine/EditorBlueprintResources/StandardMacros.IsValid` (`self.GetOwner`)
              (:`Is Not Valid`
                (set `self.Physics Enabled` true)))))))))

(event `self.ReceiveHit`
  (params (MyComp :type "PrimitiveComponent Object Reference") (Other :type "Actor Object Reference") (OtherComp :type "PrimitiveComponent Object Reference") (bSelfMoved :type Boolean) (HitLocation :type "Vector Structure") (HitNormal :type "Vector Structure") (NormalImpulse :type "Vector Structure") (Hit :type "HitResult Structure (by ref)"))
  (`parent.ReceiveHit` MyComp Other OtherComp bSelfMoved HitLocation HitNormal NormalImpulse Hit)
  (`/Engine/EditorBlueprintResources/ActorMacros.Switch Has Authority`
    (:`Authority`
      (if (not (`self.Physics Enabled`))
        (`self.Ricochet`)))))

(event `self.Ricochet`
  (set `self.Last Forward` (`KismetMathLibrary.MakeVector` (.x (`KismetMathLibrary.GetReflectionVector` (`self.Last Forward`) (`.Normal` (`GameplayStatics.BreakHitResult` (`self.Last Hit`))))) (.y (`KismetMathLibrary.GetReflectionVector` (`self.Last Forward`) (`.Normal` (`GameplayStatics.BreakHitResult` (`self.Last Hit`)))))))
  (set `self.Thrown` true))

(event `self.Deactivate Trail`)

(event `self.ReceiveTick`
  (params (DeltaSeconds :type "Float (single-precision)"))
  (`self.K2_SetActorLocation` (+ (`self.K2_GetActorLocation`) (* (`self.Last Forward`) (`self.Move Speed`) (`GameplayStatics.GetWorldDeltaSeconds`))) true) ; Sweep Spin
)

(event `self.MurderSphere.OnComponentBeginOverlap`
  (params (OverlappedComponent :type "PrimitiveComponent Object Reference") (OtherActor :type "Actor Object Reference") (OtherComp :type "PrimitiveComponent Object Reference") (OtherBodyIndex :type Integer) (bFromSweep :type Boolean) (SweepResult :type "HitResult Structure (by ref)"))
  ;[1 1 1] murder
  (if (`ActorComponent.IsActive` (`self.RotatingMovement`))
    (if (!= OtherActor (`self.Last Owner`))
      (bind _asbp_character_template (cast `/Game/Blueprints/Core/BP_Character_Template` OtherActor))
      (`|ExecutionSequence`
        (:`then_0`
          (`/Engine/EditorBlueprintResources/ActorMacros.Switch Has Authority`
            (:`Authority`
              (`self.Spin Damage` SweepResult _asbp_character_template)
              (`/Engine/EditorBlueprintResources/StandardMacros.IsValid` _asbp_character_template
                (:`Is Valid`
                  (bind _dead (`/Game/Blueprints/Core/BPI_Character.Is Dead` _asbp_character_template))
                  (if _dead
                    (`/Game/Blueprints/Core/BP_Character_Template.MC Death Impulse` _asbp_character_template (* (+ (`self.Last Forward`) (0.0 0.0 0.2)) 8000.0) (`.BoneName` (`GameplayStatics.BreakHitResult` SweepResult)))))))))
        (:`then_1`
          (`/Engine/EditorBlueprintResources/StandardMacros.Can Execute Cosmetic Events`
            (:`True`
              (`GameplayStatics.PlaySoundAtLocation` "/Game/Blueprints/GAS/Cues/Sounds/HitFlesh/A_Hit_Flesh.A_Hit_Flesh" (`.Location` (`GameplayStatics.BreakHitResult` SweepResult)) (struct) 1.0 1.0 0.0 null null null null)
              (`NiagaraFunctionLibrary.SpawnSystemAtLocation` "/Game/Blueprints/GAS/Cues/Particles/NS_BloodGPU.NS_BloodGPU" (`SceneComponent.GetSocketLocation` (`self.Item Mesh`) "Trace")))))))))

(fn `Cache Last Forward`
  (bind _ascharacter (cast `Character` (`self.Last Owner`)))
  (set `self.Last Forward` (`KismetMathLibrary.GetForwardVector` (`KismetMathLibrary.MakeRotator` 0.0 0.0 (.yaw (`.OutRotation` (`self.GetActorEyesViewPoint` _ascharacter)))))))

(fn `Spin Damage`
  (params (HitInfo :type "HitResult Structure (by ref)") (DamagedActor :type "Actor Object Reference"))
  (`GameplayStatics.ApplyPointDamage` DamagedActor 2.0 (`self.Last Forward`) HitInfo (`self.Get Damage Instigator`) self "/Game/Blueprints/Items/DamageTypes/DamageType_Polygon_Lethal_InstaKill.DamageType_Polygon_Lethal_InstaKill_C"))

(fn `UserConstructionScript`
  (`parent.UserConstructionScript`))