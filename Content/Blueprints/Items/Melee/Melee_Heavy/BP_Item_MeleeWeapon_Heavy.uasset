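; Heavy melee weapon item that adds a "steal a hammer" achievement trigger to its parent's interaction.
; When a locally controlled user interacts, it checks whether the current owner, or the last owner if there is none, is tagged AI.
; If so, it spawns an achievement progressor actor for the Hammer achievement.
; The parent interaction runs afterward in every case, and construction defers to the parent.
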(event `/Game/Primer/Primer_Interaction/BPI_Interact.Execute Interact`
  (params (User :type "Controller Object Reference"))
  (bind _returnvalue (`self.GetOwner`))
  ;[1 1 1] Steal a Hammer
  (`|ExecutionSequence`
    (:`then_0`
      (`/Engine/EditorBlueprintResources/StandardMacros.IsValid` User
        (:`Is Valid`
          (if (`Controller.IsLocalController` User)
            (`/Engine/EditorBlueprintResources/StandardMacros.IsValid` _returnvalue
              (:`Is Valid`
                (if (`self.ActorHasTag` _returnvalue "AI")
                  (`|SpawnActorFromClass` "/Game/_Guards/OnlineSubsystem/Achievements/BP_AchievementProgressor.BP_AchievementProgressor_C" (`KismetMathLibrary.Conv_VectorToTransform` (0.0 0.0 0.0)) "AlwaysSpawn" "MultiplyWithRoot" null "" "Hammer" 0 null :!label _label)))
              (:`Is Not Valid`
                (bind _last_owner (`self.Last Owner`)
                  (:`then`
                    (if (`self.ActorHasTag` _last_owner "AI")
                      (goto _label)))
                  (:`else`))))))))
    (:`then_1`
      (`parent.Execute Interact` User))))

(fn `UserConstructionScript`
  (`parent.UserConstructionScript`))