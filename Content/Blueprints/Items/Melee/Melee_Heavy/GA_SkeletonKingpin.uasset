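; Gameplay ability for the Skeleton Kingpin heavy melee weapon that repeatedly launches scythe saw blades while active.
; A looping timer fires the attack immediately and periodically, with AI avatars also playing a wide-arm montage.
; Each volley shows the weapon trail and an attached danger circle, then spawns several blades after a delay.
; The avatar gains stagger immunity until the ability ends, which unequipping the weapon triggers.
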(event `self.K2_ActivateAbility`
  (`KismetSystemLibrary.K2_SetTimerDelegate` (delegate `Launch Saw Blade`) 5.0 true)
  (`self.Launch Saw Blade`)
  (bind _item (message `/Game/Blueprints/Core/BPI_Character.Get Current Equipped Item` (`self.GetAvatarActorFromActorInfo`)))
  (bind _asbp_item_melee_weapon (cast `/Game/Blueprints/Items/Melee/BP_Item_MeleeWeapon` _item))
  (add `/Game/Blueprints/Items/BP_Item.ItemUnequip` _asbp_item_melee_weapon (delegate `ItemUnequip_Event`))
  (`AbilitySystemBlueprintLibrary.AddLooseGameplayTags` (`self.GetAvatarActorFromActorInfo`) (`BlueprintGameplayTagLibrary.MakeLiteralGameplayTagContainer` (struct :`GameplayTags` (struct :`(TagName` "Immunity.Stagger")))) true))

(event `ItemUnequip_Event`
  (params (Item :type "/Game/Blueprints/Items/BP_Item Object Reference"))
  (`self.K2_EndAbility`))

(event `Launch Saw Blade`
  (if (`Actor.ActorHasTag` (`self.GetAvatarActorFromActorInfo`) "AI")
    (`AbilityTask_PlayMontageAndWait.CreatePlayMontageAndWaitProxy` "None" "/Game/Polygon/Animations/PolygonAnims/Staff/AM_WideArm.AM_WideArm" 0.75
      (:`then`
        (`self.SawBlades`)))
    (else
      (`self.SawBlades`))))

(event `SawBlades`
  (bind _returnvalue (`self.GetAvatarActorFromActorInfo`))
  (bind _returnvalue_2 (`self.GetAvatarActorFromActorInfo`))
  (bind _item (message `/Game/Blueprints/Core/BPI_Character.Get Current Equipped Item` (`self.GetAvatarActorFromActorInfo`)))
  (bind _asbp_item_melee_weapon (cast `/Game/Blueprints/Items/Melee/BP_Item_MeleeWeapon` _item))
  (`/Game/Blueprints/Items/Melee/BP_Item_MeleeWeapon.Activate Trail` _asbp_item_melee_weapon 0.1 3.0)
  (bind _ascharacter (cast `Character` _returnvalue))
  (bind _returnvalue_3 (`|SpawnActorFromClass` "/Game/_Guards/Art/Materials/Decals/BP_DangerCircle.BP_DangerCircle_C" (`KismetMathLibrary.MakeTransform` (`Actor.K2_GetActorLocation` _returnvalue) (`KismetMathLibrary.MakeRotator` 0.0)) "AlwaysSpawn" "MultiplyWithRoot" null 3.0 _ascharacter))
  (set `self.Danger Circle` _returnvalue_3)
  (`Actor.K2_AttachToComponent` _returnvalue_3 (`Character.Mesh` _ascharacter) "None" "SnapToTarget" "KeepWorld" "KeepWorld" true)
  (`KismetSystemLibrary.Delay` 3.0)
  (for _ (range 3)
    (bind _returnvalue_4 (`|SpawnActorFromClass` "/Game/Blueprints/Items/Melee/Melee_Heavy/BP_MeleeWeapon_Scythe_SawBlade.BP_MeleeWeapon_Scythe_SawBlade_C" (`KismetMathLibrary.MakeTransform` (`Actor.K2_GetActorLocation` _returnvalue_2) (`KismetMathLibrary.MakeRotator` 0.0)) "AlwaysSpawn" "MultiplyWithRoot" null false null))
    (set `/Game/Blueprints/Items/BP_Item.Last Owner` _returnvalue_2 _returnvalue_4)))

(event `self.K2_OnEndAbility`
  (params (bWasCancelled :type Boolean))
  (`parent.K2_OnEndAbility` bWasCancelled)
  (`AbilitySystemBlueprintLibrary.RemoveLooseGameplayTags` (`self.GetAvatarActorFromActorInfo`) (`BlueprintGameplayTagLibrary.MakeLiteralGameplayTagContainer` (struct :`GameplayTags` (struct :`(TagName` "Immunity.Stagger")))) true)
  (bind _danger_circle (`self.Danger Circle`)
    (:`then`
      (`Actor.K2_DestroyActor` _danger_circle))
    (:`else`)))

(fn `K2_CanActivateAbility`
  (params (ActorInfo :type "GameplayAbilityActorInfo Structure") (Handle :type "GameplayAbilitySpecHandle Structure"))
  (returns (RelevantTags :type "GameplayTagContainer Structure") (ReturnValue :type Boolean))
  (return (struct) true))