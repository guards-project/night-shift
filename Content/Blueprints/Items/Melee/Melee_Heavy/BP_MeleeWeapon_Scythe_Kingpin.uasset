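; Kingpin scythe, a heavy melee weapon that grants the skeleton Kingpin special ability to whoever equips it.
; On equip, the server waits briefly, gives GA_SkeletonKingpin if no Ability.Special ability exists, then activates abilities with that tag.
; On unequip, the server clears the ability through the last owner's companion core component.
; Interaction is allowed only while the scythe has no owner, so it cannot be stolen.
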(event `self.On Equipped`
  (params (NewOwner :type "Actor Object Reference"))
  (bind _returnvalue (`AbilitySystemBlueprintLibrary.GetAbilitySystemComponent` (`self.GetOwner`)))
  (`parent.On Equipped` NewOwner)
  (`/Engine/EditorBlueprintResources/ActorMacros.Switch Has Authority`
    (:`Authority`
      (`KismetSystemLibrary.Delay` 0.2)
      (bind _outabilityhandles (`AbilitySystemComponent.FindAllAbilitiesWithTags` _returnvalue (`BlueprintGameplayTagLibrary.MakeLiteralGameplayTagContainer` (struct :`GameplayTags` (struct :`(TagName` "Ability.Special")))) true))
      (if (`KismetArrayLibrary.Array_IsEmpty` _outabilityhandles)
        (`AbilitySystemComponent.K2_GiveAbility` _returnvalue "/Game/Blueprints/Items/Melee/Melee_Heavy/GA_SkeletonKingpin.GA_SkeletonKingpin_C" 0 -1))
      (`AbilitySystemComponent.TryActivateAbilitiesByTag` (`AbilitySystemBlueprintLibrary.GetAbilitySystemComponent` (`self.GetOwner`)) (`BlueprintGameplayTagLibrary.MakeLiteralGameplayTagContainer` (struct :`GameplayTags` (struct :`(TagName` "Ability.Special")))) true))))

(event `self.On Unequipped`
  (`parent.On Unequipped`)
  (`/Engine/EditorBlueprintResources/ActorMacros.Switch Has Authority`
    (:`Authority`
      (bind _last_owner (`self.Last Owner`)
        (:`then`
          (`GSCCoreComponent.ClearAbility` (`GSCBlueprintFunctionLibrary.GetCompanionCoreComponent` _last_owner) "/Game/Blueprints/Items/Melee/Melee_Heavy/GA_SkeletonKingpin.GA_SkeletonKingpin_C"))
        (:`else`)))))

(fn `Get Can Interact`
  (returns (ReturnValue :type Boolean))
  ;[1 1 1] cannot steal
  (return (not (`KismetSystemLibrary.IsValid` (`self.GetOwner`)))))

(fn `UserConstructionScript`
  (`parent.UserConstructionScript`))