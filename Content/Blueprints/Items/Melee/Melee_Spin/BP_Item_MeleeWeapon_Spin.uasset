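; Spinning melee weapon item whose attack, when carried by a Polygon AI, is driven by the AI controller's target.
; On authority, equipping binds to target and arrest changes: a valid target activates the GA_Melee_Spin ability, losing it ends active item abilities.
; Arrest drops the weapon, and unequipping removes the bindings and clears the spin timer.
; TryActivate separately triggers abilities by the equipped-melee tag; the recovered/revived handler is empty.
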(event `self.On Equipped`
  (params (NewOwner :type "Actor Object Reference"))
  (`parent.On Equipped` NewOwner)
  (`/Engine/EditorBlueprintResources/ActorMacros.Switch Has Authority`
    (:`Authority`
      (bind _asbp_polygon_ai (cast `/Game/Blueprints/Core/PolygonAI/BP_Polygon_AI` NewOwner))
      (add `/Game/Blueprints/Core/BP_Character_Template.OnRecovered` _asbp_polygon_ai (delegate `OnRecovered_Event`))
      (add `/Game/Blueprints/Core/BP_Character_Template.OnRevived` _asbp_polygon_ai (delegate `OnRecovered_Event`))
      (add `/Game/Blueprints/Core/PolygonAI/BP_Polygon_AI.On Arrested Updated` _asbp_polygon_ai (delegate `On Arrested Changed`))
      (bind _asai_controller_polygon (cast `/Game/Blueprints/Core/PolygonAI/Behaviour/AI_Controller_Polygon` (`AIBlueprintHelperLibrary.GetAIController` _asbp_polygon_ai)))
      (add `/Game/Blueprints/Core/PolygonAI/Behaviour/AI_Controller_Polygon.Target Changed` _asai_controller_polygon (delegate `Target Changed_Event`))
      (`KismetSystemLibrary.Delay` 0.2)
      (`self.Target Changed_Event` _asai_controller_polygon))))

(event `OnRecovered_Event`
  (params (Character :type "/Game/Blueprints/Core/BP_Character_Template Object Reference")))

(event `On Arrested Changed`
  (params (Character :type "/Game/Blueprints/Core/BP_Character_Template Object Reference") (Arrested :type Boolean))
  (if Arrested
    (`self.Drop`)))

(event `Target Changed_Event`
  (params (Controller :type "/Game/Blueprints/Core/PolygonAI/Behaviour/AI_Controller_Polygon Object Reference"))
  (bind _returnvalue (`self.GetOwner`))
  (`/Engine/EditorBlueprintResources/StandardMacros.IsValid` _returnvalue
    (:`Is Valid`
      (bind _asbp_polygon_ai (cast `/Game/Blueprints/Core/PolygonAI/BP_Polygon_AI` _returnvalue))
      (bind _target (`/Game/Blueprints/Core/PolygonAI/Behaviour/BPI_AI.Get Target` Controller))
      (`/Engine/EditorBlueprintResources/StandardMacros.IsValid` _target
        (:`Is Valid`
          (`AbilitySystemComponent.TryActivateAbilityByClass` (`AbilitySystemBlueprintLibrary.GetAbilitySystemComponent` (`self.GetOwner`)) "/Game/Blueprints/GAS/Abilities/Attacks/GA_Melee_Spin.GA_Melee_Spin_C" true))
        (:`Is Not Valid`
          (for _array_element (`/Game/Blueprints/Items/BP_Inventory_Component.Item Ability Handles` (`self.GetComponentByClass` _asbp_polygon_ai "/Game/Blueprints/Items/BP_Inventory_Component.BP_Inventory_Component_C"))
            (bind (_bisinstance _returnvalue_2) (`AbilitySystemBlueprintLibrary.GetGameplayAbilityFromSpecHandle` (`GSCBlueprintFunctionLibrary.GetCompanionAbilitySystemComponent` _asbp_polygon_ai) _array_element))
            (bind _asga_use_item_master (cast `/Game/Blueprints/GAS/Abilities/Attacks/GA_UseItem_Master` _returnvalue_2))
            (if (`/Game/Blueprints/GAS/Abilities/Attacks/GA_UseItem_Master.Active` _asga_use_item_master)
              (`GameplayAbility.K2_EndAbility` _returnvalue_2))))))))

(event `self.On Unequipped`
  (`parent.On Unequipped`)
  (bind _last_owner (`self.Last Owner`)
    (:`then`
      (bind _asbp_polygon_ai (cast `/Game/Blueprints/Core/PolygonAI/BP_Polygon_AI` _last_owner))
      (remove `/Game/Blueprints/Core/BP_Character_Template.OnRecovered` _asbp_polygon_ai (delegate `OnRecovered_Event`))
      (remove `/Game/Blueprints/Core/BP_Character_Template.OnRevived` _asbp_polygon_ai (delegate `OnRecovered_Event`))
      (remove `/Game/Blueprints/Core/PolygonAI/BP_Polygon_AI.On Arrested Updated` _asbp_polygon_ai (delegate `On Arrested Changed`))
      (bind _asai_controller_polygon (cast `/Game/Blueprints/Core/PolygonAI/Behaviour/AI_Controller_Polygon` (`AIBlueprintHelperLibrary.GetAIController` _asbp_polygon_ai)))
      (remove `/Game/Blueprints/Core/PolygonAI/Behaviour/AI_Controller_Polygon.Target Changed` _asai_controller_polygon (`|CreateDelegate` :!event `Target Changed_Event`))
      (`KismetSystemLibrary.K2_ClearAndInvalidateTimerHandle` (`self.Spin`)))
    (:`else`)))

(event `Try Activate`
  (bind _returnvalue (`self.GetOwner`))
  (`/Engine/EditorBlueprintResources/StandardMacros.IsValid` _returnvalue
    (:`Is Valid`
      (`AbilitySystemComponent.TryActivateAbilitiesByTag` (`AbilitySystemBlueprintLibrary.GetAbilitySystemComponent` _returnvalue) (`BlueprintGameplayTagLibrary.MakeLiteralGameplayTagContainer` (struct :`GameplayTags` (struct :`(TagName` "Inventory.EquippedItem.Melee")))) true))))

(fn `UserConstructionScript`
  (`parent.UserConstructionScript`))