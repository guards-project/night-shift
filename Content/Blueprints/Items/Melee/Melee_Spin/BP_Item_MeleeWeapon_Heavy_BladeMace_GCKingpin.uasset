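; Heavy blade mace melee weapon variant for the GC Kingpin, which restyles the AI character that equips it.
; On equip by a BP_Polygon_AI, it swaps the character mesh to a red dungeon material, scales it up, then calls TryActivate after a short delay.
; Interaction is allowed only while the weapon has no valid owner, so it cannot be stolen from its wielder.
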(event `/Game/Blueprints/Items/BP_Item.On Equipped`
  (params (NewOwner :type "Actor Object Reference"))
  (`parent.On Equipped` NewOwner)
  (bind _asbp_polygon_ai (cast `/Game/Blueprints/Core/PolygonAI/BP_Polygon_AI` NewOwner))
  (bind _mesh (`Character.Mesh` _asbp_polygon_ai))
  (`PrimitiveComponent.SetMaterial` _mesh 0 "/Game/_Guards/Art/Materials/PolygonMaster/M_Polygon_Inst_Dungeon01_CharactersRed.M_Polygon_Inst_Dungeon01_CharactersRed")
  (`SceneComponent.SetWorldScale3D` _mesh (1.4 1.4 1.4))
  (`KismetSystemLibrary.Delay` 0.2)
  (`self.Try Activate`))

(fn `Get Can Interact`
  (returns (ReturnValue :type Boolean))
  ;[1 1 1] cannot steal
  (return (not (`KismetSystemLibrary.IsValid` (`self.GetOwner`)))))

(fn `UserConstructionScript`
  (`parent.UserConstructionScript`))