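; BP_Attachment is a networked item attachment actor that snaps onto a socket of a parent component.
; Parent and Socket are RepNotify variables whose handlers, along with BeginPlay, run UpdateAttachment to attach at the socket's location and rotation while keeping world scale.
; On the authority, BeginPlay binds to its owner's OnDestroyed event, apparently so the attachment destroys itself along with that owner.
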(event `self.ReceiveBeginPlay`
  (`self.Update Attachment`)
  (`/Engine/EditorBlueprintResources/ActorMacros.Switch Has Authority`
    (:`Authority`
      (add `self.OnDestroyed` (`self.GetOwner`) (`|CreateDelegate` :!event `On Parent Destroyed`)))))

(fn `Cleanup Attachment`
  (`self.K2_DestroyActor`))

(fn `On Parent Destroyed`
  (params (DestroyedActor :type "Actor Object Reference"))
  (`self.Cleanup Attachment`))

(fn `OnRep_Parent`
  (`self.Update Attachment`))

(fn `OnRep_Socket`
  (`self.Update Attachment`))

(fn `Update Attachment`
  (bind _parent (`self.Parent`)
    (:`then`
      (`self.K2_AttachToComponent` _parent (`self.Socket`) "SnapToTarget" "SnapToTarget" "KeepWorld"))
    (:`else`)))

(fn `UserConstructionScript`)