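; Attachment component that spawns cosmetic static meshes on its owner from data table rows, using either its own list or the character's config.
; Each row's mesh loads synchronously into a new collision-free component, attached at the row's bone and relative transform.
; Meshes attach to the cached character's skeletal mesh, or the owner's root if none is cached.
; An "Attachment" tag marks them so DestroyComponents can remove them from the character.
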(fn `Apply Defaults`
  (`self.Set Attachments` (`self.Attachments`)))

(fn `Apply From Character Config`
  (bind _output_get (`self.Get Character`))
  (`/Engine/EditorBlueprintResources/StandardMacros.IsValid` _output_get
    (:`Is Valid`
      (`self.Set Attachments` (`.AttachmentRows_58_FB7AD32B4419BB79705DBEB57116C71A` (break `/Game/Blueprints/Core/PolygonAI/Config/F_Character_Setup` (`/Game/Blueprints/Core/BP_Character_Template.Config Data` (`self.Character`))))))))

(fn `Destroy Components`
  (for _array_element (`Actor.GetComponentsByTag` (`self.Character`) "/Script/Engine.ActorComponent" "Attachment")
    (`/Engine/EditorBlueprintResources/StandardMacros.IsValid` _array_element
      (:`Is Valid`
        (`KismetSystemLibrary.PrintString` (`KismetSystemLibrary.GetDisplayName` _array_element))
        (`self.K2_DestroyComponent` _array_element)))))

(fn `Get Character`
  (returns (Output_Get :type "/Game/Blueprints/Core/BP_Character_Template Object Reference"))
  (bind _character (`self.Character`)
    (:`then`
      (return _character))
    (:`else`
      (bind _asbp_character_template (cast `/Game/Blueprints/Core/BP_Character_Template` (`self.GetOwner`)))
      (bind _output_get (set `self.Character` _asbp_character_template))
      (return _output_get))))

(fn `Set Attachments`
  (params (Attachments :type "Array of DataTableRowHandle Structure"))
  (locals (`L Static Mesh` :type "StaticMesh Object Reference") (`L Mesh Comp` :type "StaticMeshComponent Object Reference") (`L Attach Component` :type "SceneComponent Object Reference") (`L Attachment` :type "/Game/Blueprints/Items/Attachments/F_Attachment Structure"))
  (bind _output_get (set `self.Attachments` Attachments))
  (for _array_element _output_get
    (bind (_datatable _rowname) (break `DataTableRowHandle` _array_element))
    (`/Engine/EditorBlueprintResources/StandardMacros.IsValid` _datatable
      (:`Is Valid`
        (bind _returnvalue (`|GetDataTableRow` _datatable _rowname)
          (:`then`
            (set `local.L Attachment` _returnvalue)
            (bind _returnvalue_2 (`KismetSystemLibrary.LoadAsset_Blocking` (`.StaticMesh_5_FCEB834C46944C3F2A6C1D8589260063` (break `/Game/Blueprints/Items/Attachments/F_Attachment` _returnvalue))))
            (bind _asstatic_mesh (cast `StaticMesh` _returnvalue_2))
            (set `local.L Static Mesh` _asstatic_mesh)
            ;[1 1 1] Add Static Comp and Set Mesh
            (bind _returnvalue_3 (`|AddComponentByClass` :`self` (`self.GetOwner`) :`Class` "/Script/Engine.StaticMeshComponent"))
            (bind _output_get_2 (set `local.L Mesh Comp` _returnvalue_3))
            (`KismetArrayLibrary.Array_Add` (`self.Static Comps`) _output_get_2)
            (set `ActorComponent.ComponentTags` (`|MakeArray` "Attachment" :!type "Name") _returnvalue_3)
            (`StaticMeshComponent.SetStaticMesh` (`local.L Mesh Comp`) (`local.L Static Mesh`))
            (`PrimitiveComponent.SetCollisionEnabled` (`local.L Mesh Comp`) "NoCollision")
            ;[1 1 1] Set Root Comp and Attach
            (bind _character (`self.Character`)
              (:`then`
                (set `local.L Attach Component` (`Character.Mesh` _character)))
              (:`else`
                (set `local.L Attach Component` (`Actor.RootComponent` (`self.GetOwner`)))))
            (`SceneComponent.K2_AttachToComponent` (`local.L Mesh Comp`) (`local.L Attach Component`) (`.Bone_8_45B0C309443DDA318D42C7A85A86B5F0` (break `/Game/Blueprints/Items/Attachments/F_Attachment` (`local.L Attachment`))) "SnapToTarget" "KeepRelative" "KeepWorld" true)
            (`SceneComponent.K2_SetRelativeTransform` (`local.L Mesh Comp`) (`.RelativeTransform_12_4D1DC40345066BE8172FCCAE9D47BAAF` (break `/Game/Blueprints/Items/Attachments/F_Attachment` (`local.L Attachment`))) false false)))))))