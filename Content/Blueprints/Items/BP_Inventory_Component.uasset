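; Inventory component that manages a character's main-hand item and shield, equipping and dropping them on the server, including drops on ragdoll or stun.
; Players restore items and ammo from save data and can cache them back; other owners get a random default item or unarmed abilities.
; Equip changes propagate through OnRep handlers, which notify items and listeners and grant input-bound GAS abilities from the items, falling back to unarmed ones.
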(event `self.ReceiveBeginPlay`
  (`KismetSystemLibrary.Delay` 0.2)
  (`self.Init Inventory`))

(event `Server Give Item`
  (params (Item :type "/Game/Blueprints/Items/BP_Item Soft Class Reference"))
  (`self.Give Item` Item))

(event `Server Set Ammo`
  (params (Ammo :type Integer))
  (set `self.Persistent Ammo` Ammo)
  (`self.Update Ammo`))

(event `Init Inventory`
  (bind _returnvalue (`self.GetOwner`))
  (if (`Actor.ActorHasTag` _returnvalue "Player")
    (bind _ascharacter (cast `Character` _returnvalue))
    (cast `PlayerController` (`Pawn.GetController` _ascharacter) ; wait for player controller then init
      (:`then`
        (`self.Init Player Persistent Items`))
      (:`CastFailed`
        (`KismetSystemLibrary.K2_SetTimerDelegate` (delegate `Init Inventory`) 0.1)))
    (else
      (`KismetSystemLibrary.Delay` (`KismetMathLibrary.RandomFloatInRange` 0.5 1.5))
      (`self.Init Default Items`))))

(event `Update Ammo`
  (bind _current_item (`self.Current Item`)
    (:`then`
      (bind _returnvalue (`Actor.GetComponentByClass` _current_item "/Game/Blueprints/Items/BP_ItemAmmo.BP_ItemAmmo_C"))
      (`/Engine/EditorBlueprintResources/StandardMacros.IsValid` _returnvalue
        (:`Is Valid`
          (set `/Game/Blueprints/Items/BP_ItemAmmo.Ammo` (`KismetMathLibrary.Max` (`/Game/Blueprints/Items/BP_ItemAmmo.Ammo` _returnvalue) (`self.Persistent Ammo`)) _returnvalue))))
    (:`else`)))

(event `Server Grant Unarmed Abilities`
  (`self.Init Default Items`))

(event `Server Destroy Item`
  (params (Target :type "/Game/Blueprints/Items/BP_Item Object Reference"))
  (`self.Drop Item` Target)
  (`Actor.K2_DestroyActor` Target))

(event `Owning Client Bind Input`
  (params (InputAction :type "InputAction Object Reference") (AbilityHandle :type "GameplayAbilitySpecHandle Structure"))
  (bind _returnvalue (`GSCBlueprintFunctionLibrary.GetAbilityInputBindingComponent` (`self.GetOwner`)))
  (`GSCAbilityInputBindingComponent.ClearAbilityBindings` _returnvalue InputAction)
  (`GSCAbilityInputBindingComponent.SetInputBinding` _returnvalue InputAction "Started" AbilityHandle))

(event `self.ReceiveEndPlay`
  (params (EndPlayReason :type "EEndPlayReason Enum" :default "Destroyed"))
  (`self.Drop Item` null))

(fn `Cache Persistent Inventory`
  (locals (`L Inventory` :type "Array of /Game/Blueprints/Items/BP_Item Soft Class Reference") (`L Ammo` :type Integer :default 0) (`L Weapon Cache` :type "/Game/Blueprints/Items/BP_Item Soft Class Reference"))
  (bind (_item _shield) (`self.Get Items`))
  (`|ExecutionSequence`
    (:`then_0`
      (`/Engine/EditorBlueprintResources/StandardMacros.IsValid` _item
        (:`Is Valid`
          (bind _output (`|ConvertAsset` (`GameplayStatics.GetObjectClass` _item)))
          (set `local.L Weapon Cache` _output)
          (`KismetArrayLibrary.Array_AddUnique` (`local.L Inventory`) _output)
          (bind _returnvalue (`Actor.GetComponentByClass` _item "/Game/Blueprints/Items/BP_ItemAmmo.BP_ItemAmmo_C"))
          (`/Engine/EditorBlueprintResources/StandardMacros.IsValid` _returnvalue
            (:`Is Valid`
              (set `local.L Ammo` (`/Game/Blueprints/Items/BP_ItemAmmo.Ammo` _returnvalue)))))))
    (:`then_1`
      (`/Engine/EditorBlueprintResources/StandardMacros.IsValid` _shield
        (:`Is Valid`
          (`KismetArrayLibrary.Array_AddUnique` (`local.L Inventory`) (`|ConvertAsset` (`GameplayStatics.GetObjectClass` _shield))))))
    (:`then_2`
      (bind _player_save (`/Game/Blueprints/Core/BPFL_Guards.Get Player Save`))
      (`/Engine/EditorBlueprintResources/StandardMacros.IsValid` _player_save
        (:`Is Valid`
          (set `/Game/Blueprints/Core/PlayerSave/SaveGame_Player.Inventory` (`local.L Inventory`) _player_save)
          (set `/Game/Blueprints/Core/PlayerSave/SaveGame_Player.Ammo` (`local.L Ammo`) _player_save)
          (`GameplayStatics.SaveGameToSlot` _player_save "Player"))))))

(fn `Clear Abilities`
  (bind _returnvalue (`AbilitySystemBlueprintLibrary.GetAbilitySystemComponent` (`self.GetOwner`)))
  (bind _outabilityhandles (`AbilitySystemComponent.FindAllAbilitiesWithTags` _returnvalue (struct :`GameplayTags` (struct :`(TagName` "Inventory.EquippedItem") :`(TagName` "Inventory.Drop") :`(TagName` "Inventory.Extra"))) false))
  (for _array_element _outabilityhandles
    (`AbilitySystemComponent.ClearAbility` _returnvalue _array_element))
  ;[1 1 1] We only clear given item abilities from the player because we want the AI to continue throwing
  ; If we clear throw, the throw ends and they enter a broken state - but players should always clear given item abilities on drop
  (if (`Actor.ActorHasTag` (`self.GetOwner`) "Player")
    (for _array_element_2 (`self.Item Ability Handles`)
      (`AbilitySystemComponent.ClearAbility` _returnvalue _array_element_2))
    (`KismetArrayLibrary.Array_Clear` (`self.Item Ability Handles`))))

(fn `Drop Item`
  (params (Query :type "/Game/Blueprints/Items/BP_Item Object Reference"))
  ;[1 1 1] Note, in ABP_Polygon the shield (offhand) will override the mainhand (shield block style)
  ; If invalid, dropp all
  (`/Engine/EditorBlueprintResources/ActorComponentMacros.Switch Has Authority`
    (:`Authority`
      (`/Engine/EditorBlueprintResources/StandardMacros.IsValid` Query
        (:`Is Valid`
          (`|ExecutionSequence`
            (:`then_0`
              (if (== (`local.Query`) (`self.Current Item`))
                (set `self.Current Item` null)
                (return)))
            (:`then_1`
              (if (== (`local.Query`) (`self.Shield`))
                (set `self.Shield` null)
                (return)))))
        (:`Is Not Valid`
          (set `self.Current Item` null)
          (set `self.Shield` null))))))

(fn `Equip Item`
  (params (`New Item` :type "/Game/Blueprints/Items/BP_Item Object Reference"))
  ;[1 1 1] Note, in ABP_Polygon the shield (offhand) will override the mainhand (shield block style)
  (`/Engine/EditorBlueprintResources/ActorComponentMacros.Switch Has Authority`
    (:`Authority`
      (`/Engine/EditorBlueprintResources/StandardMacros.IsValid` `New Item`
        (:`Is Valid`
          (switch `/Game/Blueprints/Items/E_ItemType` (`/Game/Blueprints/Items/BP_Item.Item Type` `New Item`)
            (:`NewEnumerator0`
              (set `self.Current Item` (`local.New Item`)))
            (:`NewEnumerator2`
              ;;[1 1 1] Drop secondary if there is one, and equip primary
              (set `self.Shield` null)
              (set `self.Current Item` (`local.New Item`)))
            (:`NewEnumerator1`
              ;;[1 1 1] Equip shield, and drop 2 handed if held
              (set `self.Shield` (`local.New Item`))
              (bind _current_item (`self.Current Item`)
                (:`then`
                  (if (`|EnumEquality` (`/Game/Blueprints/Items/BP_Item.Item Type` _current_item) "NewEnumerator2")
                    (set `self.Current Item` null)))
                (:`else`)))))))))

(fn `Get Items`
  (returns (Item :type "/Game/Blueprints/Items/BP_Item Object Reference") (Shield :type "/Game/Blueprints/Items/BP_Item Object Reference"))
  (return (`self.Current Item`) (`self.Shield`)))

(fn `Get Persistent Inventory`
  (returns (Inventory :type "Array of /Game/Blueprints/Items/BP_Item Soft Class Reference") (Ammo :type Integer))
  (locals (`L Save` :type "/Game/Blueprints/Core/PlayerSave/SaveGame_Player Object Reference"))
  (bind _player_save (`/Game/Blueprints/Core/BPFL_Guards.Get Player Save`))
  (return (`/Game/Blueprints/Core/PlayerSave/SaveGame_Player.Inventory` _player_save) (`/Game/Blueprints/Core/PlayerSave/SaveGame_Player.Ammo` _player_save)))

(fn `Give Item`
  (params (AssetClass :type "Object Soft Class Reference"))
  (locals (`L Item` :type "/Game/Blueprints/Items/BP_Item Object Reference"))
  (bind _returnvalue (`self.GetOwner`))
  (bind _returnvalue_2 (`Actor.GetComponentByClass` (`self.Current Item`) "/Game/Blueprints/Items/BP_ItemAmmo.BP_ItemAmmo_C"))
  (bind _returnvalue_3 (`KismetSystemLibrary.LoadClassAsset_Blocking` AssetClass))
  (bind _asbp_item (castclass `/Game/Blueprints/Items/BP_Item` _returnvalue_3))
  (if (== _asbp_item (`GameplayStatics.GetObjectClass` (`self.Current Item`)))
    (`/Engine/EditorBlueprintResources/StandardMacros.IsValid` _returnvalue_2
      (:`Is Valid`
        (set `/Game/Blueprints/Items/BP_ItemAmmo.Ammo` (+ (`/Game/Blueprints/Items/BP_ItemAmmo.Ammo` _returnvalue_2) (`/Game/Blueprints/Items/BP_ItemAmmo.Default Ammo` _returnvalue_2)) _returnvalue_2))
      (:`Is Not Valid`
        (bind _returnvalue_4 (`|SpawnActorFromClass` _asbp_item (`KismetMathLibrary.Conv_VectorToTransform` (`Actor.K2_GetActorLocation` _returnvalue)) "AdjustIfPossibleButAlwaysSpawn" "SelectDefaultAtRuntime" _returnvalue false null :!label _label))
        (`|ExecutionSequence`
          (:`then_0`
            (cast `/Game/Blueprints/Items/Shield/BP_Shield_Master` _returnvalue_4
              (:`then`
                (bind _last_shield (`self.Last Shield`)
                  (:`then`
                    (bind _output_get (set `local.L Item` _last_shield))
                    (`self.Drop Item` _output_get)
                    (`Actor.K2_DestroyActor` _output_get))
                  (:`else`)))
              (:`CastFailed`
                (bind _last_item (`self.Last Item`)
                  (:`then`
                    (bind _output_get_2 (set `local.L Item` _last_item))
                    (`self.Drop Item` _output_get_2)
                    (`Actor.K2_DestroyActor` _output_get_2))
                  (:`else`)))))
          (:`then_1`
            (`self.Equip Item` _returnvalue_4)))))
    (else
      (goto _label))))

(fn `Grant Unarmed Abilities`
  (`/Engine/EditorBlueprintResources/ActorComponentMacros.Switch Has Authority`
    (:`Authority`
      (`/Engine/EditorBlueprintResources/StandardMacros.IsValid` (`self.Current Item`)
        (:`Is Not Valid`
          (`self.Clear Abilities`)
          (`self.Server Grant Abilities` (`self.Unarmed Abilities`)))))))

(fn `Init Default Items`
  (locals (`L Item` :type "/Game/Blueprints/Items/BP_Item Soft Class Reference"))
  (bind _default_items (`self.Default Items`))
  (bind (_outitem _outindex) (`KismetArrayLibrary.Array_Random` _default_items))
  (`/Engine/EditorBlueprintResources/ActorComponentMacros.Switch Has Authority`
    (:`Authority`
      (if (`KismetArrayLibrary.Array_IsValidIndex` _default_items)
        (if (>= _outindex 0)
          (bind _output_get (set `local.L Item` _outitem))
          (if (`KismetSystemLibrary.IsValidSoftClassReference` _output_get)
            (`self.Give Item` _output_get)
            (else
              (`self.Grant Unarmed Abilities` :!label _label)))
          (else
            (goto _label)))
        (else
          (goto _label))))))

(fn `Init Player Persistent Items`
  (bind _ascharacter (cast `Character` (`self.GetOwner`)))
  (if (`Pawn.IsLocallyControlled` _ascharacter)
    (bind _player_save (`/Game/Blueprints/Core/BPFL_Guards.Get Player Save`))
    (`/Engine/EditorBlueprintResources/StandardMacros.IsValid` _player_save
      (:`Is Valid`
        (bind (_inventory _ammo) (`self.Get Persistent Inventory`))
        (if (`KismetArrayLibrary.Array_IsEmpty` _inventory)
          (`self.Server Grant Unarmed Abilities`)
          (else
            (for _array_element _inventory
              (`self.Server Give Item` _array_element))
            (`self.Server Set Ammo` _ammo))))
      (:`Is Not Valid`
        (`KismetSystemLibrary.K2_SetTimerDelegate` (`|CreateDelegate` :!event `Init Player Persistent Items`) 0.1)))))

(fn `On Owner Ragdoll`
  ;[1 1 1] Always drop items when KO / Dead
  (bind (_item _shield) (`self.Get Items`))
  (`|ExecutionSequence`
    (:`then_0`
      (`/Engine/EditorBlueprintResources/StandardMacros.IsValid` _item
        (:`Is Valid`
          (if (`/Game/Blueprints/Items/BP_Item.Can Drop from Ragdoll` _item)
            (`self.Drop Item` _item)))))
    (:`then_1`
      (`/Engine/EditorBlueprintResources/StandardMacros.IsValid` _shield
        (:`Is Valid`
          (if (`/Game/Blueprints/Items/BP_Item.Can Drop from Ragdoll` _shield)
            (`self.Drop Item` _shield)))))))

(fn `On Owner Stun`
  ;[1 1 1] Some items stay in hand when standing stunned
  (bind (_item _shield) (`self.Get Items`))
  (`|ExecutionSequence`
    (:`then_0`
      (`/Engine/EditorBlueprintResources/StandardMacros.IsValid` _item
        (:`Is Valid`
          (if (`/Game/Blueprints/Items/BP_Item.Can Drop from Stun` _item)
            (`self.Drop Item` _item)))))
    (:`then_1`
      (`/Engine/EditorBlueprintResources/StandardMacros.IsValid` _shield
        (:`Is Valid`
          (if (`/Game/Blueprints/Items/BP_Item.Can Drop from Stun` _shield)
            (`self.Drop Item` _shield)))))))

(fn `OnRep_Current Item`
  (`|ExecutionSequence`
    (:`then_0`
      (bind _last_item (`self.Last Item`)
        (:`then`
          (`/Game/Blueprints/Items/BP_Item.On Unequipped` _last_item))
        (:`else`)))
    (:`then_1`
      (set `self.Last Item` (`self.Current Item`)) ; not replicated
      (`self.Current Item`
        (:`then`
          (`/Game/Blueprints/Items/BP_Item.On Equipped` (`self.Current Item`) (`self.GetOwner`)) ; manages anim sets and other states
          (`/Engine/EditorBlueprintResources/ActorComponentMacros.Switch Has Authority`
            (:`Authority`
              ;[1 1 1] Clear all abilities and grant all
              (`self.Clear Abilities`)
              (`|ExecutionSequence`
                (:`then_0`
                  (bind _current_item (`self.Current Item`)
                    (:`then`
                      (`self.Server Grant Abilities` (`/Game/Blueprints/Items/BP_Item.Granted Abilities` _current_item) true))
                    (:`else`)))
                (:`then_1`
                  (bind _shield (`self.Shield`)
                    (:`then`
                      (`self.Server Grant Abilities` (`/Game/Blueprints/Items/BP_Item.Granted Abilities` _shield) true))
                    (:`else`)))))))
        (:`else`
          (`self.Grant Unarmed Abilities`))))
    (:`then_2`
      (`self.OnEquippedItemChanged` (`self.Current Item`) (`self.Shield`)))))

(fn `OnRep_Shield`
  (`|ExecutionSequence`
    (:`then_0`
      (bind _last_shield (`self.Last Shield`)
        (:`then`
          (`/Game/Blueprints/Items/BP_Item.On Unequipped` _last_shield))
        (:`else`)))
    (:`then_1`
      (set `self.Last Shield` (`self.Shield`)) ; not replicated
      (`self.Shield`
        (:`then`
          (`/Game/Blueprints/Items/BP_Item.On Equipped` (`self.Shield`) (`self.GetOwner`)) ; manages anim sets and other states
          (`/Engine/EditorBlueprintResources/ActorComponentMacros.Switch Has Authority`
            (:`Authority`
              ;[1 1 1] REMOVED BECAUSE SHIELD ABILITIES BREAK REGULAR ONES
              ; Clear all abilities and grant all
              (`self.Grant Unarmed Abilities`)
              (`|ExecutionSequence`
                (:`then_0`
                  (bind _current_item (`self.Current Item`)
                    (:`then`
                      (`self.Server Grant Abilities` (`/Game/Blueprints/Items/BP_Item.Granted Abilities` _current_item)))
                    (:`else`)))
                (:`then_1`
                  (bind _shield (`self.Shield`)
                    (:`then`
                      (`self.Server Grant Abilities` (`/Game/Blueprints/Items/BP_Item.Granted Abilities` _shield)))
                    (:`else`)))))))
        (:`else`
          (`self.Current Item`
            (:`then`)
            (:`else`
              (`self.Grant Unarmed Abilities`))))))
    (:`then_2`
      (`self.OnEquippedItemChanged` (`self.Current Item`) (`self.Shield`)))))

(fn `Server Grant Abilities`
  (params (`Abilities Input Map` :type "Map of GameplayAbility Soft Class Reference to InputAction Object Reference (by ref)") (`From Item` :type Boolean))
  (bind _asgscability_system_component (cast `GSCAbilitySystemComponent` (`AbilitySystemBlueprintLibrary.GetAbilitySystemComponent` (`self.GetOwner`))))
  (bind _keys (`BlueprintMapLibrary.Map_Keys` (`local.Abilities Input Map`)))
  (for _array_element _keys
    (bind _returnvalue (`KismetSystemLibrary.LoadClassAsset_Blocking` _array_element))
    (bind _asgameplay_ability (castclass `GameplayAbility` _returnvalue))
    (bind _returnvalue_2 (`GSCAbilitySystemComponent.GrantAbility` _asgscability_system_component _asgameplay_ability false))
    (`self.Owning Client Bind Input` (`BlueprintMapLibrary.Map_Find` (`local.Abilities Input Map`) _array_element) _returnvalue_2)
    (if `From Item`
      (`KismetArrayLibrary.Array_Add` (`self.Item Ability Handles`) _returnvalue_2))))