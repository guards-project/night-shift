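; Nail bomb grenade item that deals damage by scattering bolt projectiles instead of applying it directly.
; DealDamage spawns Shots BP_Projectile_Bolt actors at the bomb's location, owned by it and passing on its instigator.
; Each bolt gets a random yaw around the full circle and a random pitch between horizontal and Pitch.
; Optional debug arrows re-roll the random direction, so they do not match the bolts' actual paths.
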(fn `Deal Damage`
  (bind _returnvalue (`self.K2_GetActorLocation`))
  (bind _returnvalue_2 (`KismetMathLibrary.GreaterGreater_VectorRotator` (`KismetMathLibrary.MakeVector` 1.0) (`KismetMathLibrary.MakeRotator` 0.0 (`KismetMathLibrary.RandomFloatInRange` 0.0 (`self.Pitch`)) (`KismetMathLibrary.RandomFloatInRange` 0.0 360.0))))
  ;[1 1 1] Fire X Shots
  (for _ (range (`self.Shots`))
    (`|SpawnActorFromClass` "/Game/Blueprints/Items/Ranged/BP_Projectile_Bolt.BP_Projectile_Bolt_C" (`KismetMathLibrary.MakeTransform` _returnvalue (`KismetMathLibrary.Conv_VectorToRotator` _returnvalue_2)) "AlwaysSpawn" "SelectDefaultAtRuntime" self (`self.Get Instigator`))
    ;[1 1 1] Debug
    (if (`self.Debug`)
      (`KismetSystemLibrary.DrawDebugArrow` _returnvalue (+ _returnvalue (* _returnvalue_2 500.0)) 10.0 (struct :`R` 0.814847 :`G` 0.021219 :`B` 0.021219 :`A` 1.0) 20.0 5.0))))

(fn `UserConstructionScript`
  (`parent.UserConstructionScript`))