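; Throwable grenade item that explodes on impact when its fuse time is zero or less, otherwise after a fuse delay from the throw.
; The server triggers detonation from the parent's throw and hit events, then destroys the actor after a post-explosion delay.
; MCExplode hides the grenade and disables collision, applies radial damage and optional impulse on authority, and spawns Niagara and sound effects where cosmetic events can run.
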(event `self.Execute Gameplay Thrown Hit Cue`
  (`parent.Execute Gameplay Thrown Hit Cue`)
  (set `self.Can Ever Interact` false)
  (`/Engine/EditorBlueprintResources/ActorMacros.Switch Has Authority`
    (:`Authority`
      (if (`self.Should Explode on Impact`)
        (`/Engine/EditorBlueprintResources/StandardMacros.DoOnce` false
          (:`Completed`
            (`self.Server Init Explode`)))))))

(event `self.Throw Item`
  (params (Location :type "Vector Structure") (Impulse :type "Vector Structure") (Torque :type "Vector Structure") (Thrown :type Boolean))
  (`parent.Throw Item` Location Impulse Torque Thrown)
  (set `self.Can Ever Interact` false)
  (`/Engine/EditorBlueprintResources/ActorMacros.Switch Has Authority`
    (:`Authority`
      (if (not (`self.Should Explode on Impact`))
        (`KismetSystemLibrary.Delay` (`self.Fuse Time`))
        (`self.Server Init Explode`)))))

(event `Server Init Explode`
  (`self.MC Explode` (+ (`.Location` (`GameplayStatics.BreakHitResult` (`self.Last Hit`))) (0.0 0.0 5.0)))
  (`KismetSystemLibrary.Delay` (`self.Post Explode Lifetime`))
  (`self.K2_DestroyActor`))

(event `MC Explode`
  (params (Location :type "Vector Structure"))
  (`self.SetActorEnableCollision` false)
  (`self.SetActorHiddenInGame` true)
  (`|ExecutionSequence`
    (:`then_0`
      ;[1 1 1] Server gameplay
      (`/Engine/EditorBlueprintResources/ActorMacros.Switch Has Authority`
        (:`Authority`
          (`self.Deal Damage`)
          (`self.Do Impulse`))))
    (:`then_1`
      ;[1 1 1] Client visuals
      (`/Engine/EditorBlueprintResources/StandardMacros.Can Execute Cosmetic Events`
        (:`True`
          (`self.Do Client Explosion FX` Location))))))

(fn `Deal Damage`
  (if (> (`self.Damage`) 0.0)
    (`GameplayStatics.ApplyRadialDamage` :`BaseDamage` (`self.Damage`) :`Origin` (+ (`self.K2_GetActorLocation`) (`KismetMathLibrary.MakeVector` 0.0 0.0 (`self.Damage Origin Z Offset`))) :`DamageRadius` (`self.Damage Radius`) :`DamageTypeClass` (`self.Damage Type Class`) :`DamageCauser` self :`InstigatedByController` (`Pawn.GetController` (`self.Get Instigator`)) :`bDoFullDamage` (`self.Do Full Damage`) :`DamagePreventionChannel` "ECC_GameTraceChannel6")))

(fn `Do Client Explosion FX`
  (params (InputPin :type "Vector Structure"))
  (`NiagaraFunctionLibrary.SpawnSystemAtLocation` (`self.Explode Niagara`) InputPin)
  (`GameplayStatics.PlaySoundAtLocation` (`self.Explode Sound`) InputPin (struct) 1.0 1.0 0.0 null null null null))

(fn `Do Impulse`
  (if (`self.Should Impulse`)
    (`RadialForceComponent.FireImpulse` (`self.RadialForce`))))

(fn `Get Instigator`
  (returns (Instigator :type "Pawn Object Reference"))
  (bind _last_owner (`self.Last Owner`))
  (`/Engine/EditorBlueprintResources/StandardMacros.IsValid` _last_owner
    (:`Is Valid`
      (return (`Actor.Instigator` _last_owner)))
    (:`Is Not Valid`
      (return null))))

(fn `Should Explode on Impact`
  (returns (`On Impact` :type Boolean))
  (return (<= (`self.Fuse Time`) 0.0)))

(fn `UserConstructionScript`
  (`parent.UserConstructionScript`))