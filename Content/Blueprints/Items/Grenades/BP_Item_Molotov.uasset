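; Molotov grenade item that sets nearby characters alight and leaves lingering fire on the ground.
; On explosion it runs the parent logic, then traces downward (with persistent debug drawing) to spawn BP_LingerDamage_Fire.
; DealDamage replaces the parent version, stunning characters within DamageRadius, applying GE_OnFire and recording them.
; It calls DealFireDamage for lethal-type point damage and guard stagger on living victims, then starts a looping timer.
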(event `Deal Fire Damage`
  (for _array_element (`self.Characters On Fire`)
    (`/Engine/EditorBlueprintResources/StandardMacros.IsValid` _array_element
      (:`Is Valid`
        (bind _dead (message `/Game/Blueprints/Core/BPI_Character.Is Dead` _array_element))
        (if (not _dead)
          (`GameplayStatics.ApplyPointDamage` _array_element 1.0 (`KismetMathLibrary.MakeVector` 0.0 0.0 1.0) (`GameplayStatics.MakeHitResult` false) (`self.GetInstigatorController`) self "/Game/Blueprints/Items/DamageTypes/DamageType_Polygon_Lethal.DamageType_Polygon_Lethal_C")
          (bind _asbp_character_template (cast `/Game/Blueprints/Core/BP_Character_Template` _array_element))
          (`AbilitySystemComponent.BP_ApplyGameplayEffectToSelf` :`self` (`/Game/Blueprints/Core/BP_Character_Template.GSCAbilitySystem` _asbp_character_template) :`GameplayEffectClass` "/Game/Blueprints/GAS/Effects/GE_GuardStagger.GE_GuardStagger_C"))))))

(event `self.Server Init Explode`
  (bind _returnvalue (`self.K2_GetActorLocation`))
  (`parent.Server Init Explode`)
  (bind (_outhit _returnvalue_2) (`KismetSystemLibrary.LineTraceSingle` :`Start` _returnvalue :`End` (+ _returnvalue (0.0 0.0 -500.0)) :`TraceChannel` "TraceTypeQuery2" :`DrawDebugType` "Persistent"))
  (if _returnvalue_2
    (`|SpawnActorFromClass` "/Game/Blueprints/Items/Grenades/BP_LingerDamage_Fire.BP_LingerDamage_Fire_C" (`KismetMathLibrary.Conv_VectorToTransform` (`.Location` (`GameplayStatics.BreakHitResult` _outhit))) "AlwaysSpawn" "MultiplyWithRoot" null null)))

(fn `Deal Damage`
  (bind _outactors (`KismetSystemLibrary.SphereOverlapActors` (`self.K2_GetActorLocation`) (`self.Damage Radius`) (`|MakeArray` "ObjectTypeQuery3" :!type "EObjectTypeQuery Enum") "/Game/Blueprints/Core/BP_Character_Template.BP_Character_Template_C"))
  (for _array_element _outactors
    (bind _asbp_character_template (cast `/Game/Blueprints/Core/BP_Character_Template` _array_element))
    (`/Game/Blueprints/Core/BP_Character_Template.Stun` _asbp_character_template)
    (`KismetArrayLibrary.Array_Add` (`self.Characters On Fire`) _asbp_character_template)
    (`AbilitySystemComponent.BP_ApplyGameplayEffectToSelf` :`self` (`AbilitySystemBlueprintLibrary.GetAbilitySystemComponent` _array_element) :`GameplayEffectClass` "/Game/Blueprints/GAS/Effects/GE_OnFire.GE_OnFire_C"))
  (`self.Deal Fire Damage`)
  (`KismetSystemLibrary.K2_SetTimerDelegate` (`|CreateDelegate` :!event `Deal Fire Damage`) 1.0 true))

(fn `UserConstructionScript`
  (`parent.UserConstructionScript`))