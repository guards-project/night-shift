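; Lingering fire area, from the grenade item set, that sets overlapping characters on fire and damages them over time.
; While active, overlap start records each character and applies the GE_OnFire gameplay effect.
; An authority-only looping timer deals point damage to recorded living characters, who stay listed after leaving the area.
; After a delay the area stops igniting and switches off its Niagara fire, then destroys itself shortly after.
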(event `self.ReceiveBeginPlay`
  (`parent.ReceiveBeginPlay`)
  (`/Engine/EditorBlueprintResources/ActorMacros.Switch Has Authority`
    (:`Authority`
      (`KismetSystemLibrary.K2_SetTimerDelegate` (delegate `Deal Fire Damage`) 1.0 true)
      (`KismetSystemLibrary.Delay` 9.0)
      (set `self.Active` false)
      (`self.MC Fire Off`)
      (`KismetSystemLibrary.Delay` 2.0)
      (`self.K2_DestroyActor`))))

(event `Deal Fire Damage`
  (for _array_element (`self.Characters On Fire`)
    (`/Engine/EditorBlueprintResources/StandardMacros.IsValid` _array_element
      (:`Is Valid`
        (bind _dead (message `/Game/Blueprints/Core/BPI_Character.Is Dead` _array_element))
        (if (not _dead)
          (`GameplayStatics.ApplyPointDamage` _array_element 1.0 (`KismetMathLibrary.MakeVector` 0.0 0.0 1.0) (`GameplayStatics.MakeHitResult` false) (`self.GetInstigatorController`) self "/Game/Blueprints/Items/DamageTypes/DamageType_Polygon_Lethal.DamageType_Polygon_Lethal_C"))))))

(event `MC Fire Off`
  (`ActorComponent.Deactivate` (`self.Niagara`)))

(fn `On Overlap Ended`
  (params (Character :type "/Game/Blueprints/Core/BP_Character_Template Object Reference"))
  (`parent.On Overlap Ended` Character))

(fn `On Overlap Started`
  (params (Character :type "/Game/Blueprints/Core/BP_Character_Template Object Reference"))
  (`parent.On Overlap Started` Character)
  (if (`self.Active`)
    (`KismetArrayLibrary.Array_Add` (`self.Characters On Fire`) (`local.Character`))
    (`AbilitySystemComponent.BP_ApplyGameplayEffectToSelf` :`self` (`AbilitySystemBlueprintLibrary.GetAbilitySystemComponent` (`local.Character`)) :`GameplayEffectClass` "/Game/Blueprints/GAS/Effects/GE_OnFire.GE_OnFire_C")))

(fn `UserConstructionScript`
  (`parent.UserConstructionScript`))