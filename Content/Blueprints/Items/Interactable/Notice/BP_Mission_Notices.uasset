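; BP_Mission_Notices is a mission Blueprint that tracks how many notices in the level have been interacted with.
; On BeginPlay, the authority gathers every BP_Interact_Notice actor and sets the target count to the number found.
; It binds to each notice's CanInteractChanged event and increments the current count whenever one reports it can no longer be interacted with.
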(event `self.ReceiveBeginPlay`
  (`parent.ReceiveBeginPlay`)
  (`/Engine/EditorBlueprintResources/ActorMacros.Switch Has Authority`
    (:`Authority`
      (bind _outactors (`GameplayStatics.GetAllActorsOfClass` "/Game/Blueprints/Items/Interactable/Notice/BP_Interact_Notice.BP_Interact_Notice_C"))
      (bind _output_get (set `self.Notices` _outactors))
      (set `self.Target Count` (`KismetArrayLibrary.Array_Length` _output_get))
      (for _array_element _output_get
        (add `/Game/Primer/Primer_Interaction/BP_Interactable.Can Interact Changed` _array_element (delegate `Can Interact Changed_Event`))))))

(event `Can Interact Changed_Event`
  (params (`Can Interact` :type Boolean))
  (if (not `Can Interact`)
    (set `self.Current Count` (+ (`self.Current Count`) 1))))

(fn `UserConstructionScript`
  (`parent.UserConstructionScript`))