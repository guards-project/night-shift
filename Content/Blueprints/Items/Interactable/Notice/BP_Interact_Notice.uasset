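; Interactable notice that shows as a transparent placeholder with a hidden widget until a player uses it.
; A one-shot interaction locks it on the server and awards capped duty coins; outside the hub, the local user also gets achievement progress and a UMG event.
; In the hub, ResetInteraction re-arms it.
; On the server it destroys itself when its parent actor is destroyed or, for fracture actors, fractured or kicked.
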(event `self.ReceiveBeginPlay`
  (bind _returnvalue (`self.GetAttachParentActor`))
  (`parent.ReceiveBeginPlay`)
  (`self.On Can Interact Changed` (`self.Can Interact`))
  (`/Engine/EditorBlueprintResources/StandardMacros.IsValid` _returnvalue
    (:`Is Valid`
      (`/Engine/EditorBlueprintResources/ActorMacros.Switch Has Authority`
        (:`Authority`
          (add `self.OnDestroyed` _returnvalue (delegate `OnDestroyed_Event_0`))
          (bind _asbp_fracture_actor (cast `/Game/Blueprints/Fracture/FractureCore/BP_FractureActor` _returnvalue))
          (add `/Game/Blueprints/Fracture/FractureCore/BP_FractureActor.Fractured` _asbp_fracture_actor (delegate `Fractured_Event`))
          (add `/Game/Blueprints/Fracture/FractureCore/BP_FractureActor.KickEvent` _asbp_fracture_actor (delegate `KickEvent_Event`)))))))

(event `OnDestroyed_Event_0` :!signature `self.OnDestroyed`
  (params (DestroyedActor :type "Actor Object Reference"))
  (`self.K2_DestroyActor`))

(event `Fractured_Event`
  (params (Actor :type "/Game/Blueprints/Fracture/FractureCore/BP_FractureActor Object Reference"))
  (remove `/Game/Blueprints/Fracture/FractureCore/BP_FractureActor.KickEvent` Actor (`|CreateDelegate` :!event `KickEvent_Event`))
  (`self.K2_DestroyActor`))

(event `KickEvent_Event`
  (params (Actor :type "/Game/Blueprints/Fracture/FractureCore/BP_FractureActor Object Reference"))
  (remove `/Game/Blueprints/Fracture/FractureCore/BP_FractureActor.Fractured` Actor (`|CreateDelegate` :!event `Fractured_Event`))
  (`self.K2_DestroyActor`))

(event `Reset Interaction`
  (if (`/Game/Blueprints/Core/BPFL_Guards.Is HUB`)
    (set `self.Can Interact` true)
    (goto _label :!via `Reset`)))

(event `/Game/Primer/Primer_Interaction/BPI_Interact.Execute Interact`
  (params (User :type "Controller Object Reference"))
  (`parent.Execute Interact` User)
  (`/Engine/EditorBlueprintResources/StandardMacros.DoOnce` false :!label _label
    (:`Completed`
      (`|ExecutionSequence`
        (:`then_0`
          (`/Engine/EditorBlueprintResources/ActorMacros.Switch Has Authority`
            (:`Authority`
              (set `self.Can Interact` false)
              (`/Game/Blueprints/Core/Score/BPFL_Score.Add Score` (`PlayerState.GetPlayerName` (`Controller.PlayerState` User)) "Coins_Duty" (`KismetMathLibrary.Min` (`self.Coins`) 50)))))
        (:`then_1`
          (if (not (`/Game/Blueprints/Core/BPFL_Guards.Is HUB`))
            (`/Engine/EditorBlueprintResources/StandardMacros.IsValid` User
              (:`Is Valid`
                (if (`Controller.IsLocalPlayerController` User)
                  (`self.Increment User Stat`)
                  (`/Game/Primer/Primer_UMGEvent/BPFL_Primer_UMGEvent.Create UMG Event` (`self.UMG Event`)))))))))))

(event `self.On Can Interact Changed`
  (params (CanInteract :type Boolean))
  (`parent.On Can Interact Changed` CanInteract)
  (`PrimitiveComponent.SetMaterial` (`self.StaticMesh`) 0 (select `bool` (`self.Can Interact`) :`true` "/Game/_Guards/Art/Materials/Transparent/M_TransparentBasic_Inst.M_TransparentBasic_Inst" :!type "MaterialInterface Object Reference")) ; to default
  (`SceneComponent.SetHiddenInGame` (`self.BP_ActorWidgetComponent`) (`self.Can Interact`) true))

(event `Increment User Stat`
  ;[1 1 1] Achievement Progress Setup
  (`|SpawnActorFromClass` "/Game/_Guards/OnlineSubsystem/Achievements/BP_AchievementProgressor.BP_AchievementProgressor_C" (`KismetMathLibrary.Conv_VectorToTransform` (0.0 0.0 0.0)) "AlwaysSpawn" "MultiplyWithRoot" null "Player_Notices" "Notice" 1 null))

(fn `Update Widget`
  (`/Game/_Guards/UserInterface/ActorWidget/BP_ActorWidgetComponent.Set Widget Actor` (`self.BP_ActorWidgetComponent`)))

(fn `UserConstructionScript`
  (`parent.UserConstructionScript`)
  (`self.Update Widget`))