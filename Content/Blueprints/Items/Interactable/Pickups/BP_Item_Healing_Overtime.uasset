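; Interactable pickup item that, by its name, heals the player over time.
; Its only logic is the Get Can Interact override, which allows interaction while one float attribute on player 0's Ability System Component is below another, presumably health against max health.
; Event graph and construction script add nothing of their own, and the healing effect itself is not defined in these graphs.
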(fn `Get Can Interact`
  (returns (ReturnValue :type Boolean))
  (bind _returnvalue (`AbilitySystemBlueprintLibrary.GetAbilitySystemComponent` (`GameplayStatics.GetPlayerPawn` 0)))
  (return (< (`.ReturnValue` (`AbilitySystemBlueprintLibrary.GetFloatAttributeFromAbilitySystemComponent` _returnvalue (struct :`AttributeName` "Health" :`Attribute` "/Script/GASCompanion.GSCAttributeSet:Health" :`AttributeOwner` "/Script/CoreUObject.Class'\"/Script/GASCompanion.GSCAttributeSet\"'"))) (`.ReturnValue` (`AbilitySystemBlueprintLibrary.GetFloatAttributeFromAbilitySystemComponent` _returnvalue (struct :`AttributeName` "MaxHealth" :`Attribute` "/Script/GASCompanion.GSCAttributeSet:MaxHealth" :`AttributeOwner` "/Script/CoreUObject.Class'\"/Script/GASCompanion.GSCAttributeSet\"'"))))))

(fn `UserConstructionScript`
  (`parent.UserConstructionScript`))