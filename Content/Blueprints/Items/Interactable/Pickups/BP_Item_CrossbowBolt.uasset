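; Crossbow bolt pickup that adds one round of ammo to a crossbow in the interacting player's inventory.
; On interact it plays a pickup sound, then on authority increments the crossbow's ammo if below max and optionally destroys itself.
; The interact check allows pickup only when player 0's inventory item is a crossbow with room for ammo, regardless of who interacts.
; Interaction is instant within a short fixed distance.
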(event `/Game/Primer/Primer_Interaction/BPI_Interact.Execute Interact`
  (params (User :type "Controller Object Reference"))
  (bind _returnvalue (`Controller.K2_GetPawn` User))
  (`GameplayStatics.PlaySoundAtLocation` "/Game/Fantasy_Interface_SFX/cue/BowPickup_Sound.BowPickup_Sound" (`self.K2_GetActorLocation`) (struct) 1.0 1.0 0.0 null null null null)
  (`/Engine/EditorBlueprintResources/ActorMacros.Switch Has Authority`
    (:`Authority`
      (`/Engine/EditorBlueprintResources/StandardMacros.IsValid` _returnvalue
        (:`Is Valid`
          (bind _item (`/Game/Blueprints/Items/BP_Inventory_Component.Get Items` (`self.GetComponentByClass` _returnvalue "/Game/Blueprints/Items/BP_Inventory_Component.BP_Inventory_Component_C")))
          (bind _asbp_item_ranged_weapon_crossbow (cast `/Game/Blueprints/Items/Ranged/BP_Item_RangedWeapon_Crossbow` _item))
          (bind _bp_itemammo (`/Game/Blueprints/Items/Ranged/BP_Item_RangedWeapon.BP_ItemAmmo` _asbp_item_ranged_weapon_crossbow))
          (bind _ammo (`/Game/Blueprints/Items/BP_ItemAmmo.Ammo` _bp_itemammo))
          (if (< _ammo (`/Game/Blueprints/Items/BP_ItemAmmo.Max Ammo` _bp_itemammo))
            (set `/Game/Blueprints/Items/BP_ItemAmmo.Ammo` (+ _ammo 1) _bp_itemammo)
            (if (`self.Destroy on Pickup`)
              (`self.K2_DestroyActor`))))))))

(fn `Get Can Interact`
  (returns (ReturnValue :type Boolean))
  (bind _returnvalue (`GameplayStatics.GetPlayerPawn` 0))
  (bind _returnvalue_2 (`self.GetComponentByClass` _returnvalue "/Game/Blueprints/Items/BP_Inventory_Component.BP_Inventory_Component_C"))
  (`/Engine/EditorBlueprintResources/StandardMacros.IsValid` _returnvalue
    (:`Is Valid`
      (`/Engine/EditorBlueprintResources/StandardMacros.IsValid` _returnvalue_2
        (:`Is Valid`
          (bind _item (`/Game/Blueprints/Items/BP_Inventory_Component.Get Items` _returnvalue_2))
          (bind _asbp_item_ranged_weapon_crossbow (cast `/Game/Blueprints/Items/Ranged/BP_Item_RangedWeapon_Crossbow` _item)
            (:`then`
              (bind _bp_itemammo (`/Game/Blueprints/Items/Ranged/BP_Item_RangedWeapon.BP_ItemAmmo` _asbp_item_ranged_weapon_crossbow))
              (return (< (`/Game/Blueprints/Items/BP_ItemAmmo.Ammo` _bp_itemammo) (`/Game/Blueprints/Items/BP_ItemAmmo.Max Ammo` _bp_itemammo))))
            (:`CastFailed`
              _)))
        (:`Is Not Valid`
          _)))
    (:`Is Not Valid`
      _))
  (return false))

(fn `Get Interact Distance`
  (returns (Distance :type "Float (double-precision)"))
  (return 250.0))

(fn `Get Interact Duration`
  (returns (Duration :type "Float (double-precision)"))
  (return 0.0))

(fn `UserConstructionScript`
  (`parent.UserConstructionScript`))