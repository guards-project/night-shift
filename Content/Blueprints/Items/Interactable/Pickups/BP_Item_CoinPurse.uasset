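; Coin purse pickup that grants coins to the player who interacts with it, scaled up in its construction script.
; On interact, the local player gets a UI event, a "Confiscated" achievement progressor and coins added to their save.
; The server separately records the coins as score under the player's name, then destroys the purse, which plays a coin sound on destruction.
; The parent's interact logic is deliberately left unconnected.
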(event `/Game/Primer/Primer_Interaction/BPI_Interact.Execute Interact`
  (params (User :type "Controller Object Reference"))
  (`|ExecutionSequence`
    (:`then_0`
      ;[1 1 1] Local Player
      (if (`Controller.IsLocalPlayerController` User)
        (`/Game/Primer/Primer_UMGEvent/BPFL_Primer_UMGEvent.Create UMG Event` (`self.UMG Event`))
        (`|SpawnActorFromClass` "/Game/_Guards/OnlineSubsystem/Achievements/BP_AchievementProgressor.BP_AchievementProgressor_C" (`KismetMathLibrary.Conv_VectorToTransform` (0.0 0.0 0.0)) "AlwaysSpawn" "MultiplyWithRoot" null "Player_CoinBags" "Confiscated" 1 null)
        (bind _player_save (`/Game/Blueprints/Core/BPFL_Guards.Get Player Save`))
        (`/Game/Blueprints/Core/PlayerSave/SaveGame_Player.Edit Coins` _player_save (`self.Coins`) "Coin Purse")))
    (:`then_1`
      ;[1 1 1] Server
      (`/Engine/EditorBlueprintResources/ActorMacros.Switch Has Authority`
        (:`Authority`
          (`|ExecutionSequence`
            (:`then_0`
              (bind _playerstate (`Controller.PlayerState` User)
                (:`then`
                  (`/Game/Blueprints/Core/Score/BPFL_Score.Add Score` (`PlayerState.GetPlayerName` _playerstate) "Coins" (`self.Coins`)))
                (:`else`)))
            (:`then_1`
              (`self.K2_DestroyActor`))))))))

(event `self.ReceiveDestroyed`
  (`GameplayStatics.PlaySoundAtLocation` "/Game/Fantasy_Interface_SFX/cue/Coin_and_Purse_06_Cue.Coin_and_Purse_06_Cue" (`self.K2_GetActorLocation`) (struct) 1.0 1.0 0.0 null null null null))

(fn `UserConstructionScript`
  (`parent.UserConstructionScript`)
  (`self.SetActorScale3D` (3.0 3.0 3.0)))