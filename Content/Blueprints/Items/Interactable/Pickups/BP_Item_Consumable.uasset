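; Base-style consumable pickup item that a character drinks once on interaction, with prompt text and widget reflecting whether it can be used.
; On authority, it applies a configurable gameplay effect, an attack-stop effect and a drink-animation effect through the user's Ability System Component.
; MCHold then disables interaction and physics, cosmetically attaches the item to DrinkSocket, and on authority applies delayed point damage to the drinker before destroying the item.
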(event `/Game/Primer/Primer_Interaction/BPI_Interact.Execute Interact`
  (params (User :type "Controller Object Reference"))
  (bind _returnvalue (`Controller.K2_GetPawn` User))
  (`/Engine/EditorBlueprintResources/ActorMacros.Switch Has Authority`
    (:`Authority`
      (`/Engine/EditorBlueprintResources/StandardMacros.DoOnce` false
        (:`Completed`
          (`self.Apply Effects` (`AbilitySystemBlueprintLibrary.GetAbilitySystemComponent` _returnvalue))
          (bind _ascharacter (cast `Character` _returnvalue))
          (`self.MC Hold` _ascharacter))))))

(event `MC Hold`
  (params (Target :type "Character Object Reference"))
  (set `self.Target` Target)
  (set `self.Can Ever Interact` false)
  (set `self.Physics Enabled` false)
  (`self.Update Physics`)
  (`|ExecutionSequence`
    (:`then_0`
      (`/Engine/EditorBlueprintResources/StandardMacros.Can Execute Cosmetic Events`
        (:`True`
          (`self.K2_AttachToComponent` (`Character.Mesh` (`self.Target`)) "DrinkSocket" "SnapToTarget" "SnapToTarget" "KeepWorld"))))
    (:`then_1`
      (`/Engine/EditorBlueprintResources/ActorMacros.Switch Has Authority`
        (:`Authority`
          (`KismetSystemLibrary.Delay` 1.0)
          (`GameplayStatics.ApplyPointDamage` (`self.Target`) (`self.Damage amount`) (`KismetMathLibrary.MakeVector` 0.0) (`GameplayStatics.MakeHitResult` false) null self "/Game/Blueprints/Items/DamageTypes/DamageType_Polygon.DamageType_Polygon_C")
          (`KismetSystemLibrary.Delay` (`self.Life after Use`))
          (`self.K2_DestroyActor`))))))

(fn `Apply Effects`
  (params (InputPin :type "AbilitySystemComponent Object Reference"))
  (bind _returnvalue (`AbilitySystemComponent.MakeEffectContext` InputPin))
  (bind _level (`self.Level`))
  (`AbilitySystemComponent.BP_ApplyGameplayEffectToSelf` InputPin (`self.Gameplay Effect Class`) _level _returnvalue) ; do unique effect
  (`AbilitySystemComponent.BP_ApplyGameplayEffectToSelf` InputPin "/Game/Blueprints/GAS/Effects/GE_StopAttacks.GE_StopAttacks_C" _level _returnvalue) ; stop abilities
  (`AbilitySystemComponent.BP_ApplyGameplayEffectToSelf` :`self` InputPin :`GameplayEffectClass` "/Game/Blueprints/GAS/Effects/GE_DrinkAnim.GE_DrinkAnim_C") ; instant cue drink
)

(fn `Get Always Show Widget`
  (returns (`Always Show` :type Boolean))
  (return true))

(fn `Get Interact Text`
  (returns (Text :type Text))
  (bind _returnvalue (`/Game/Primer/Primer_Interaction/BPI_Interact.Get Can Interact`))
  (return (select `bool` _returnvalue :`false` (`self.No Interact Text`) :`true` (`self.Interact Text`))))

(fn `Get Interact Widget Class`
  (returns (`Widget Class` :type "/Game/Primer/Primer_Interaction/UI/W_Interact_Master Soft Class Reference"))
  (bind _returnvalue (`/Game/Primer/Primer_Interaction/BPI_Interact.Get Can Interact`))
  (if _returnvalue
    (bind _widget_class (`parent.Get Interact Widget Class`))
    (return _widget_class)
    (else
      (return "/Game/Primer/Primer_Interaction/UI/W_Interact_nonInteractable.W_Interact_nonInteractable_C"))))

(fn `UserConstructionScript`
  (`parent.UserConstructionScript`))