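; Replicated ammo component for items, letting an item of the same class top up the user's held item when consumed.
; On the server, Consume moves this item's Ammo into the equipped item's component up to MaxAmmo and keeps the remainder.
; It returns true on a merge, or false when the held item is missing or a different class.
; Ammo's RepNotify broadcasts the change through AmmoUpdated.
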(fn `Consume`
  (params (User :type "Controller Object Reference"))
  (returns (Consumed :type Boolean))
  (locals (`L Remainder` :type Integer))
  ;[1 1 1] When Interacting with this weapon
  ; If its a knife, Add 1 ammo to the held item, don't pickup and destroy the knife instead
  ; Otherwise, if its a different weapon, continue the normal flow (drop held item, and pickup other item)
  (if (`Actor.HasAuthority` (`self.GetOwner`))
    (bind _item (message `/Game/Blueprints/Core/BPI_Character.Get Current Equipped Item` (`Controller.K2_GetPawn` (`local.User`))))
    (`/Engine/EditorBlueprintResources/StandardMacros.IsValid` _item
      (:`Is Valid`
        (if (== (`GameplayStatics.GetObjectClass` (`self.GetOwner`)) (`GameplayStatics.GetObjectClass` _item))
          (bind _returnvalue (`Actor.GetComponentByClass` _item "BP_ItemAmmo_C"))
          (bind _returnvalue_2 (+ (`/Game/Blueprints/Items/BP_ItemAmmo.Ammo` _returnvalue) (`self.Ammo`)))
          (bind _max_ammo (`/Game/Blueprints/Items/BP_ItemAmmo.Max Ammo` _returnvalue))
          (set `local.L Remainder` (- _returnvalue_2 _max_ammo))
          (set `/Game/Blueprints/Items/BP_ItemAmmo.Ammo` (`KismetMathLibrary.Min` _returnvalue_2 _max_ammo) _returnvalue)
          (set `self.Ammo` (`KismetMathLibrary.Max` (`local.L Remainder`))) ; set self to remaining
          (return true)
          (else
            _)))
      (:`Is Not Valid`
        _))
    (return false)))

(fn `OnRep_Ammo`
  (`self.Ammo Updated` self (`self.Ammo`)))