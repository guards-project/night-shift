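; Weapon wall slot that displays an item as a child actor, or a transparent ghost mesh while locked.
; Interacting with the same item in hand unlocks all matching slots and saves it; otherwise, unlocked slots sell it for coins, discounted by saved count up to half price.
; The server gives items, tops up ammo or destroys deposited non-ammo items, while the local client updates save data, coins and visuals.
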(event `self.ReceiveBeginPlay`
  (`self.Configure Item`))

(event `Configure Item`
  (bind _childactor (`ChildActorComponent.ChildActor` (`self.Item`))
    (:`then`
      (`self.SetActorEnableCollision` _childactor false)
      (`self.Load Save Data`))
    (:`else`
      (`KismetSystemLibrary.Delay` 0.2)
      (`self.Configure Item`))))

(event `/Game/Primer/Primer_Interaction/BPI_Interact.Execute Interact`
  (params (User :type "Controller Object Reference"))
  (bind _returnvalue (`Controller.K2_GetPawn` User))
  (bind _last_held_item (`self.Last Held Item`))
  (bind (_same_item _item) (`self.Is Player Holding Same Item` _returnvalue))
  (bind _output (`|ConvertAsset` (`self.Item Class`)))
  (`parent.Execute Interact` User)
  ;[1 1 1] server side
  (`|ExecutionSequence`
    (:`then_0`
      (`/Engine/EditorBlueprintResources/ActorMacros.Switch Has Authority`
        (:`Authority`
          (set `self.Last Held Item` _item)
          (if _same_item
            (`KismetSystemLibrary.Delay` 0.2) ; allow client side first
            (bind _last_held_item_2 (`self.Last Held Item`)
              (:`then`
                (bind (_is_ammo_based _can_pickup) (`self.Pickup Ammo` _last_held_item_2))
                (if _is_ammo_based
                  (if _can_pickup
                    (bind _asbp_character_template (cast `/Game/Blueprints/Core/BP_Character_Template` _returnvalue :!label _label))
                    (`/Game/Blueprints/Items/BP_Inventory_Component.Server Give Item` (`/Game/Blueprints/Core/BP_Character_Template.BP_Inventory_Component` _asbp_character_template) (`|ConvertAsset` (`self.Item Class`))))
                  (else
                    (`/Game/Blueprints/Items/BP_Item.Drop` _last_held_item)
                    (`self.K2_DestroyActor` _last_held_item))))
              (:`else`))
            (else
              (`KismetSystemLibrary.Delay` 0.2)
              (goto _label))))))
    (:`then_1`
      ;[1 1 1] client side
      (`GameplayStatics.PlaySoundAtLocation` "/Game/_Guards/Audio/Sounds/A_EquipmentFoley_Cue.A_EquipmentFoley_Cue" (`self.K2_GetActorLocation`) (struct) 1.0 1.0 0.0 null null null null)
      (if (`Controller.IsLocalPlayerController` User)
        (if (`self.Is Player Holding Same Item` (`Controller.K2_GetPawn` User))
          (`self.Unlock` true)
          (bind _player_save (`/Game/Blueprints/Core/BPFL_Guards.Get Player Save`))
          (`/Game/Blueprints/Core/PlayerSave/SaveGame_Player.Give Item` _player_save _output)
          (else
            (`self.Spend Gold`)
            (bind _player_save_2 (`/Game/Blueprints/Core/BPFL_Guards.Get Player Save`))
            (`/Game/Blueprints/Core/PlayerSave/SaveGame_Player.Take Item` _player_save_2 _output)))
        (`self.Cache Can Afford`)
        (`self.Updated`)))))

(event `/Game/Primer/Primer_Interaction/BPI_Interact.Start Focus`
  (`self.Cache Can Afford` :!label _label_2)
  (`self.Updated`))

(event `/Game/Primer/Primer_Interaction/BPI_Interact.Stop Focus`
  (goto _label_2))

(fn `Cache Can Afford`
  (bind _player_save (`/Game/Blueprints/Core/BPFL_Guards.Get Player Save`))
  (`/Engine/EditorBlueprintResources/StandardMacros.IsValid` _player_save
    (:`Is Valid`
      (set `self.Can Afford` (>= (`/Game/Blueprints/Core/PlayerSave/SaveGame_Player.Coins` _player_save) (`self.Get Cost`))))))

(fn `Get Can Interact`
  (returns (ReturnValue :type Boolean))
  (bind _same_item (`self.Is Player Holding Same Item` (`Controller.K2_GetPawn` (`GameplayStatics.GetPlayerController` 0))))
  (if (`self.Unlocked`)
    (return (or (`self.Can Afford`) _same_item)) ; can interact if unlocked\ni.e. drop current pickup new\nOR slot current onto wall
    (else
      (return _same_item) ; can add same item to wall slot
    )))

(fn `Get Cost`
  (returns (Cost :type Integer) (Discount :type Integer))
  (bind _cost (defaults `Object` (`self.Item Class`)))
  (bind _returnvalue (/ _cost 2))
  (bind _player_save (`/Game/Blueprints/Core/BPFL_Guards.Get Player Save`))
  (`/Engine/EditorBlueprintResources/StandardMacros.IsValid` _player_save
    (:`Is Valid`
      (bind (_value _returnvalue_2) (`BlueprintMapLibrary.Map_Find` (`/Game/Blueprints/Core/PlayerSave/SaveGame_Player.UnlockedItems` _player_save) (`|ConvertAsset` (`self.Item Class`))))
      (if _returnvalue_2
        (if (== _value 0)
          (return 0 0)
          (else
            (bind _returnvalue_3 (* (- _value 1) 10))
            (return (`KismetMathLibrary.Max` (- _cost _returnvalue_3) _returnvalue) (`KismetMathLibrary.Min` _returnvalue_3 _returnvalue))))
        (else
          (return (defaults `Object` (`self.Item Class`)) 0))))))

(fn `Get Highlight Meshes`
  (returns (Array :type "Array of PrimitiveComponent Object Reference"))
  (bind _childactor (`ChildActorComponent.ChildActor` (`self.Item`)))
  (`/Engine/EditorBlueprintResources/StandardMacros.IsValid` _childactor
    (:`Is Valid`
      (bind _asbp_item (cast `/Game/Blueprints/Items/BP_Item` _childactor))
      (return (`/Game/Blueprints/Items/BP_Item.Get Highlight Meshes` _asbp_item)))
    (:`Is Not Valid`
      (return (`|MakeArray` null :!type "PrimitiveComponent Object Reference")))))

(fn `Is Player Holding Same Item`
  (params (Pawn :type "Pawn Object Reference"))
  (returns (`Same Item` :type Boolean) (Item :type "/Game/Blueprints/Items/BP_Item Object Reference"))
  (bind _item (message `/Game/Blueprints/Core/BPI_Character.Get Current Equipped Item` Pawn))
  (`/Engine/EditorBlueprintResources/StandardMacros.IsValid` _item
    (:`Is Valid`
      (bind _asbp_item (cast `/Game/Blueprints/Items/BP_Item` _item))
      (return (== (`GameplayStatics.GetObjectClass` _item) (`self.Item Class`)) _asbp_item))
    (:`Is Not Valid`
      (return false null))))

(fn `Load Save Data`
  (locals (`L Item` :type "/Game/Blueprints/Items/BP_Item Object Reference"))
  (bind _player_save (`/Game/Blueprints/Core/BPFL_Guards.Get Player Save`))
  (`/Engine/EditorBlueprintResources/StandardMacros.IsValid` _player_save
    (:`Is Valid`
      (bind (_value _returnvalue) (`BlueprintMapLibrary.Map_Find` (`/Game/Blueprints/Core/PlayerSave/SaveGame_Player.UnlockedItems` _player_save) (`|ConvertAsset` (`self.Item Class`))))
      (set `self.Unlocked` (or _returnvalue (`self.Starter Item`)))
      (set `self.Num Times Bought` _value)
      (`self.Update Visual`))
    (:`Is Not Valid`
      (`KismetSystemLibrary.K2_SetTimerDelegate` (`|CreateDelegate` :!event `Load Save Data`) 0.2))))

(fn `Lock`
  (params (Propogate :type Boolean))
  (set `self.Unlocked` false)
  (`self.Update Visual`)
  (if Propogate
    (bind _outactors (`GameplayStatics.GetAllActorsOfClass` "BP_UnlockItem_C"))
    (for _array_element _outactors
      (if (== (`/Game/Blueprints/Items/WeaponWall/BP_UnlockItem.Item Class` _array_element) (`self.Item Class`))
        (`self.Lock` _array_element false)))))

(fn `Pickup Ammo`
  (params (Item :type "Actor Object Reference"))
  (returns (`Is Ammo Based` :type Boolean) (`Can Pickup` :type Boolean))
  (bind _returnvalue (`self.GetComponentByClass` Item "/Game/Blueprints/Items/BP_ItemAmmo.BP_ItemAmmo_C"))
  (`/Engine/EditorBlueprintResources/StandardMacros.IsValid` _returnvalue
    (:`Is Valid`
      (return true (<= (+ (`/Game/Blueprints/Items/BP_ItemAmmo.Ammo` _returnvalue) (`/Game/Blueprints/Items/BP_ItemAmmo.Default Ammo` _returnvalue)) (`/Game/Blueprints/Items/BP_ItemAmmo.Max Ammo` _returnvalue))))
    (:`Is Not Valid`
      (return false false))))

(fn `Spend Gold`
  (bind _player_save (`/Game/Blueprints/Core/BPFL_Guards.Get Player Save`))
  (`/Game/Blueprints/Core/PlayerSave/SaveGame_Player.Edit Coins` _player_save (* (`self.Get Cost`) -1) "Buy Item")
  (`self.Cache Can Afford`))

(fn `Unlock`
  (params (Propagate :type Boolean))
  (set `self.Unlocked` true)
  (`self.Update Visual`)
  (if Propagate
    (bind _outactors (`GameplayStatics.GetAllActorsOfClass` "BP_UnlockItem_C"))
    (for _array_element _outactors
      (if (== (`/Game/Blueprints/Items/WeaponWall/BP_UnlockItem.Item Class` _array_element) (`self.Item Class`))
        (`self.Unlock` _array_element false)))))

(fn `Update Interact Bounds`
  (bind _box (`self.Box`))
  (bind _childactor (`ChildActorComponent.ChildActor` (`self.Item`))
    (:`then`
      (bind _asbp_item (cast `/Game/Blueprints/Items/BP_Item` _childactor))
      (bind _interactbox (`/Game/Blueprints/Items/BP_Item.InteractBox` _asbp_item))
      (`BoxComponent.SetBoxExtent` _box (* (`BoxComponent.BoxExtent` _interactbox) (`self.Bound Scale`)) true)
      (`SceneComponent.K2_SetRelativeTransform` _box (`SceneComponent.GetRelativeTransform` _interactbox) false false))
    (:`else`)))

(fn `Update Item`
  (`ChildActorComponent.SetChildActorClass` (`self.Item`) (`self.Item Class`))
  (`self.Update Interact Bounds`))

(fn `Update Visual`
  (locals (`L Item` :type "/Game/Blueprints/Items/BP_Item Object Reference"))
  (bind _l_item (`local.L Item`))
  (bind _staticmesh (`self.StaticMesh`))
  (bind _childactor (`ChildActorComponent.ChildActor` (`self.Item`))
    (:`then`
      (bind _asbp_item (cast `/Game/Blueprints/Items/BP_Item` _childactor))
      (set `local.L Item` _asbp_item)
      (if (`self.Unlocked`)
        (`SceneComponent.SetHiddenInGame` (`self.Item`) false false)
        (`ActorComponent.Deactivate` (`self.K2_GetComponentsByClass` (`local.L Item`) "/Script/Engine.AudioComponent"))
        (`/Game/Blueprints/Items/BP_Item.Set White Fill` _l_item false)
        (`/Game/Blueprints/Items/BP_Item.Set Mesh Highlight` _l_item false)
        (`SceneComponent.SetVisibility` (`self.StaticMesh`) false false)
        (else
          (`StaticMeshComponent.SetStaticMesh` _staticmesh (`StaticMeshComponent.StaticMesh` (`/Game/Blueprints/Items/BP_Item.Item Mesh` _asbp_item)))
          (for _index (range (`PrimitiveComponent.GetNumMaterials` _staticmesh))
            (`PrimitiveComponent.SetMaterial` _staticmesh _index "/Game/_Guards/Art/Materials/Transparent/M_Transparent_WeaponWall.M_Transparent_WeaponWall") ; ghost
          )
          (`SceneComponent.SetHiddenInGame` (`self.Item`) true false)
          (`ActorComponent.Deactivate` (`self.K2_GetComponentsByClass` (`local.L Item`) "/Script/Engine.AudioComponent"))
          (`SceneComponent.SetVisibility` (`self.StaticMesh`) true false))))
    (:`else`)))

(fn `UserConstructionScript`
  (`parent.UserConstructionScript`)
  (`self.Update Item`))