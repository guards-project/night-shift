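; Goblin Shaman staff weapon that grants temporary invulnerability to nearby allies through the Gameplay Ability System.
; ApplyBuff sphere-overlaps pawns within BuffRadius, excluding the owner, and applies GE_Invulnerable_Goblin to living, non-KO teammates that are not Shamans.
; A DoOnce, reset on each cast, fires the replicated MCBuff event so the Niagara blast spawns once, only when an ally receives the buff.
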(event `self.Apply Buff`
  ;[0.008023 0.402 1] Apply Buff
  (`/Engine/EditorBlueprintResources/StandardMacros.IsValid` (`self.GetOwner`)
    (:`Is Valid`
      (`self.Reset Once Pop`)
      (bind _outactors (`KismetSystemLibrary.SphereOverlapActors` (`self.K2_GetActorLocation`) (`self.Buff Radius`) (`|MakeArray` "ObjectTypeQuery3" :!type "EObjectTypeQuery Enum") "/Game/Blueprints/Core/BP_Character_Template.BP_Character_Template_C" (`|MakeArray` (`self.GetOwner`))))
      (for _array_element _outactors
        (bind _dead (message `/Game/Blueprints/Core/BPI_Character.Is Dead` _array_element))
        (bind _ko (message `/Game/Blueprints/Core/BPI_Character.Is KO` _array_element))
        (if (and (not (or _dead _ko)) (`/Game/Blueprints/Core/Components/BP_Team_Component.Same Team` (`self.My Team`) (`self.GetComponentByClass` _array_element "/Game/Blueprints/Core/Components/BP_Team_Component.BP_Team_Component_C")))
          (bind _asbp_character_template (cast `/Game/Blueprints/Core/BP_Character_Template` _array_element))
          (bind (_config_datatable _config_rowname) (break `DataTableRowHandle` (`/Game/Blueprints/Core/BP_Character_Template.Config` _asbp_character_template)))
          (if (!= _config_rowname "Goblin_Shaman")
            (`AbilitySystemComponent.BP_ApplyGameplayEffectToSelf` :`self` (`AbilitySystemBlueprintLibrary.GetAbilitySystemComponent` _array_element) :`GameplayEffectClass` "/Game/Blueprints/GAS/Effects/GE_Invulnerable_Goblin.GE_Invulnerable_Goblin_C")
            (`/Engine/EditorBlueprintResources/StandardMacros.DoOnce` false :!label _label
              (:`Completed`
                (`self.MC Buff` (`self.K2_GetActorLocation`))))))))))

(event `Reset Once Pop`
  ;[0.008023 0.402 1] Apply Buff
  (goto _label :!via `Reset`))

(event `self.MC Buff`
  (params (Location :type "Vector Structure") (Component :type "SceneComponent Object Reference"))
  ;[0.3226 0.03711 0.5938] Replicated
  (`NiagaraFunctionLibrary.SpawnSystemAtLocation` "/Game/_Guards/Art/Particles/NS_InvulnerableBlast.NS_InvulnerableBlast" Location))

(fn `UserConstructionScript`
  (`parent.UserConstructionScript`))