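; Base staff weapon that lets an AI owner pulse a buff on a looping timer, with the buff effect left empty in ApplyBuff.
; Equipping on authority starts buffing and sets whether the AI can move; KO, death or unequip stops it, recovery resumes it and arrest drops the staff.
; A replicated BuffingActive flag toggles FX, audio and light through its RepNotify, and destruction spawns a networked smoke pop.
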(event `self.On Unequipped`
  ;[0.008023 0.402 1] Apply Buff
  (`parent.On Unequipped`)
  (`self.Set Buffing` false)
  (`self.Unbind Events`))

(event `self.On Equipped`
  (params (NewOwner :type "Actor Object Reference"))
  ;[0.008023 0.402 1] Apply Buff
  (`parent.On Equipped` NewOwner)
  (`/Engine/EditorBlueprintResources/ActorMacros.Switch Has Authority`
    (:`Authority`
      (set `self.My Team` (`self.GetComponentByClass` (`self.GetOwner`) "/Game/Blueprints/Core/Components/BP_Team_Component.BP_Team_Component_C"))
      (`self.Set Buffing` true)
      (bind _asbp_polygon_ai (cast `/Game/Blueprints/Core/PolygonAI/BP_Polygon_AI` (`self.GetOwner`)))
      (`/Game/Blueprints/Core/BP_Character_Template.Auth Set Can Move` _asbp_polygon_ai (`self.Can Move while Buffing`))
      (`self.Bind Events`))))

(event `Apply Buff`
  ;[0.008023 0.402 1] Apply Buff
)

(event `Bind Events`
  ;[0.008023 0.402 1] Apply Buff
  (bind _asbp_polygon_ai (cast `/Game/Blueprints/Core/PolygonAI/BP_Polygon_AI` (`self.GetOwner`)))
  (add `/Game/Blueprints/Core/BP_Character_Template.OnDied` _asbp_polygon_ai (delegate `OnDown`))
  (add `/Game/Blueprints/Core/BP_Character_Template.OnKO` _asbp_polygon_ai (delegate `OnDown`))
  (add `/Game/Blueprints/Core/BP_Character_Template.OnRecovered` _asbp_polygon_ai (delegate `OnRecovered_Event`))
  (add `/Game/Blueprints/Core/PolygonAI/BP_Polygon_AI.On Arrested Updated` _asbp_polygon_ai (delegate `On Arrested Updated_Event`)))

(event `OnDown`
  (params (Character :type "/Game/Blueprints/Core/BP_Character_Template Object Reference"))
  ;[0.008023 0.402 1] Apply Buff
  (`self.Set Buffing` false))

(event `On Arrested Updated_Event`
  (params (Character :type "/Game/Blueprints/Core/BP_Character_Template Object Reference") (Arrested :type Boolean))
  ;[0.008023 0.402 1] Apply Buff
  (if Arrested
    (`self.Drop`)))

(event `OnRecovered_Event`
  (params (Character :type "/Game/Blueprints/Core/BP_Character_Template Object Reference"))
  ;[0.008023 0.402 1] Apply Buff
  (`self.Set Buffing` true))

(event `self.ReceiveDestroyed`
  ;[0.008023 0.402 1] Apply Buff
  (`/Game/Blueprints/Core/BPFL_Guards.Create Networked FX` (`self.K2_GetActorLocation`) "/Game/Shooter_VFXPack/Particles/HitsAndExplosions/NS_SmokePop.NS_SmokePop" "/Game/_Guards/Audio/Sounds/A_SmokePop.A_SmokePop"))

(event `MC Buff`
  (params (Location :type "Vector Structure") (Component :type "SceneComponent Object Reference"))
  ;[0.3226 0.03711 0.5938] Replicated
)

(fn `On Buffing Active Changed`
  (bind _pointlight (`self.PointLight`))
  (if (`self.Buffing Active`)
    (`ActorComponent.Activate` (`self.FX`) false)
    (`ActorComponent.Activate` (`self.Audio`) false)
    (`ActorComponent.Activate` _pointlight false)
    (`SceneComponent.SetVisibility` _pointlight true false)
    (else
      (`ActorComponent.Deactivate` (`self.Audio`))
      (`ActorComponent.Deactivate` _pointlight)
      (`ActorComponent.Deactivate` (`self.FX`))
      (`SceneComponent.SetVisibility` _pointlight false false))))

(fn `OnRep_Buffing Active`
  (`self.On Buffing Active Changed`))

(fn `Set Buffing`
  (params (Condition :type Boolean))
  (if Condition
    ;[1 1 1] Only enemy can enable this
    (bind _asbp_polygon_ai (cast `/Game/Blueprints/Core/PolygonAI/BP_Polygon_AI` (`self.GetOwner`)))
    (`/Game/Blueprints/Core/BP_Character_Template.Auth Set Can Move` _asbp_polygon_ai (`self.Can Move while Buffing`))
    (bind _returnvalue (`KismetSystemLibrary.K2_SetTimerDelegate` (`|CreateDelegate` :!event `Apply Buff`) (`self.Buff Frequency`) true))
    (set `self.Buff Handle` _returnvalue)
    (set `self.Buffing Active` true)
    (`self.Apply Buff`)
    (else
      (`KismetSystemLibrary.K2_ClearAndInvalidateTimerHandle` (`self.Buff Handle`))
      (set `self.Buffing Active` false)
      (bind _last_owner (`self.Last Owner`)
        (:`then`
          (bind _asbp_polygon_ai_2 (cast `/Game/Blueprints/Core/PolygonAI/BP_Polygon_AI` _last_owner))
          (`/Game/Blueprints/Core/BP_Character_Template.Auth Set Can Move` _asbp_polygon_ai_2 true))
        (:`else`)))))

(fn `Unbind Events`
  (bind _last_owner (`self.Last Owner`)
    (:`then`
      (bind _asbp_polygon_ai (cast `/Game/Blueprints/Core/PolygonAI/BP_Polygon_AI` _last_owner))
      (remove `/Game/Blueprints/Core/BP_Character_Template.OnDied` _asbp_polygon_ai (`|CreateDelegate` :!event `OnDown`))
      (remove `/Game/Blueprints/Core/BP_Character_Template.OnKO` _asbp_polygon_ai (`|CreateDelegate` :!event `OnDown`))
      (remove `/Game/Blueprints/Core/PolygonAI/BP_Polygon_AI.On Arrested Updated` _asbp_polygon_ai (`|CreateDelegate` :!event `On Arrested Updated_Event`))
      (remove `/Game/Blueprints/Core/BP_Character_Template.OnRecovered` _asbp_polygon_ai (`|CreateDelegate` :!event `OnRecovered_Event`)))
    (:`else`)))

(fn `UserConstructionScript`
  (`parent.UserConstructionScript`))