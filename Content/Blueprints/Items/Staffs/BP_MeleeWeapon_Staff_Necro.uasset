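; Necromancer staff weapon whose buff revives dead or knocked-out same-team characters within BuffRadius of the staff.
; ApplyBuff sphere-overlaps for characters, sends revive messages, then calls a replicated event for revive effect, sound and the owner's attack montage.
; Buff state changes toggle a necromancer particle attached to an AI owner's capsule, setting a short timer if no owner is valid yet.
; Destruction spawns a networked smoke pop.
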(event `self.Apply Buff`
  ;[0.008023 0.402 1] Apply Buff
  (`/Engine/EditorBlueprintResources/StandardMacros.IsValid` (`self.GetOwner`)
    (:`Is Valid`
      (bind _outactors (`KismetSystemLibrary.SphereOverlapActors` (`self.K2_GetActorLocation`) (`self.Buff Radius`) (`|MakeArray` "ObjectTypeQuery3" "ObjectTypeQuery4" "ObjectTypeQuery7" :!type "EObjectTypeQuery Enum") "/Game/Blueprints/Core/BP_Character_Template.BP_Character_Template_C" (`|MakeArray` (`self.GetOwner`))))
      (for _array_element _outactors
        (bind _dead (message `/Game/Blueprints/Core/BPI_Character.Is Dead` _array_element))
        (bind _ko (message `/Game/Blueprints/Core/BPI_Character.Is KO` _array_element))
        (if (and (`/Game/Blueprints/Core/Components/BP_Team_Component.Same Team` (`self.My Team`) (`self.GetComponentByClass` _array_element "/Game/Blueprints/Core/Components/BP_Team_Component.BP_Team_Component_C")) (or _dead _ko))
          (message `/Game/Blueprints/Core/BPI_Character.Revive` _array_element)
          (bind _ascharacter (cast `Character` _array_element))
          (`self.MC Buff` (`SceneComponent.K2_GetComponentLocation` (`Character.Mesh` _ascharacter)) (`Character.CapsuleComponent` _ascharacter)))))))

(event `self.ReceiveDestroyed`
  ;[0.008023 0.402 1] Apply Buff
  (`/Game/Blueprints/Core/BPFL_Guards.Create Networked FX` (`self.K2_GetActorLocation`) "/Game/Shooter_VFXPack/Particles/HitsAndExplosions/NS_SmokePop.NS_SmokePop" "/Game/_Guards/Audio/Sounds/A_SmokePop.A_SmokePop"))

(event `self.MC Buff`
  (params (Location :type "Vector Structure") (Component :type "SceneComponent Object Reference"))
  ;[0.3226 0.03711 0.5938] Replicated
  (`GameplayStatics.SpawnEmitterAttached` "/Game/StylishVFXCollection/4_Particles/MagicSquare/MagicSquare_03/P_Revive.P_Revive" Component "None" (0.0 0.0 -85.0) (struct) (1.0 1.0 1.0) "SnapToTarget")
  (`GameplayStatics.PlaySoundAtLocation` "/Game/_Guards/Audio/Sounds/A_Revive_Cue.A_Revive_Cue" Location (struct) 1.0 1.0 0.0 null null null null)
  (bind _ascharacter (cast `Character` (`self.GetOwner`)))
  (`Character.PlayAnimMontage` _ascharacter "/Game/Polygon/Animations/PolygonAnims/Halberd/AM_Attack_Halberd_02.AM_Attack_Halberd_02" 1.0 "None"))

(fn `On Buffing Active Changed`
  (bind _returnvalue (`self.GetOwner`))
  (`parent.On Buffing Active Changed`)
  (if (`self.Buffing Active`)
    (`/Engine/EditorBlueprintResources/StandardMacros.IsValid` _returnvalue
      (:`Is Valid`
        (bind _asbp_polygon_ai (cast `/Game/Blueprints/Core/PolygonAI/BP_Polygon_AI` _returnvalue))
        (`self.Set Necromancer Particle` true (`Character.CapsuleComponent` _asbp_polygon_ai)))
      (:`Is Not Valid`
        (`KismetSystemLibrary.K2_SetTimerDelegate` (`|CreateDelegate` :!event `On Buffing Active Changed`) 0.5)))
    (else
      (bind _last_owner (`self.Last Owner`)
        (:`then`
          (cast `/Game/Blueprints/Core/PolygonAI/BP_Polygon_AI` _last_owner)
          (`self.Set Necromancer Particle` false))
        (:`else`)))))

(fn `Set Necromancer Particle`
  (params (Condition :type Boolean) (AttachToComponent :type "SceneComponent Object Reference"))
  (if Condition
    (bind _returnvalue (`GameplayStatics.SpawnEmitterAttached` "/Game/StylishVFXCollection/4_Particles/MagicSquare/MagicSquare_03/P_Necromancer.P_Necromancer" AttachToComponent "None" (0.0 0.0 -85.0) (struct) (1.0 1.0 1.0) "SnapToTarget"))
    (set `self.Necro Effect` _returnvalue)
    (else
      (bind _necro_effect (`self.Necro Effect`)
        (:`then`
          (`ActorComponent.Deactivate` _necro_effect))
        (:`else`)))))

(fn `UserConstructionScript`
  (`parent.UserConstructionScript`))