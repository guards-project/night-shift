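; Throwable gas barrel item that, when thrown or shot, flies erratically like a rocket, then explodes.
; The server enables physics and plays the GasForce timeline, scaled to FlyTime, for thrust along the barrel's up axis.
; Tick adds random torque, hits bounce it off surfaces, and a fire trail and audio follow physics state.
; After FlyTime it explodes once with multicast effects, radial damage and force, then destroys itself.
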(event `self.ReceiveBeginPlay`
  (`parent.ReceiveBeginPlay`)
  (`TimelineComponent.SetPlayRate` (`self.gas force`) (/ 1.0 (`self.Fly Time`))))

(event `self.Throw Item`
  (params (Location :type "Vector Structure") (Impulse :type "Vector Structure") (Torque :type "Vector Structure") (Thrown :type Boolean))
  (`parent.Throw Item` Location Impulse Torque Thrown)
  (`self.Set Can Fly`))

(event `self.ReceiveHit`
  (params (MyComp :type "PrimitiveComponent Object Reference") (Other :type "Actor Object Reference") (OtherComp :type "PrimitiveComponent Object Reference") (bSelfMoved :type Boolean) (HitLocation :type "Vector Structure") (HitNormal :type "Vector Structure") (NormalImpulse :type "Vector Structure") (Hit :type "HitResult Structure (by ref)"))
  (if (`self.Physics Enabled`)
    (`PrimitiveComponent.AddImpulse` (`self.Item Mesh`) (* HitNormal 800.0) "None" true)
    (set `self.Desired Rotation` (`KismetMathLibrary.Conv_VectorToRotator` NormalImpulse))
    (`self.Start Rand Torque Timer`)))

(event `self.ReceivePointDamage`
  (params (Damage :type "Float (single-precision)") (DamageType :type "DamageType Object Reference") (HitLocation :type "Vector Structure") (HitNormal :type "Vector Structure") (HitComponent :type "PrimitiveComponent Object Reference") (BoneName :type Name) (ShotFromDirection :type "Vector Structure") (InstigatedBy :type "Controller Object Reference") (DamageCauser :type "Actor Object Reference") (HitInfo :type "HitResult Structure (by ref)"))
  (`self.Set Can Fly`)
  (`PrimitiveComponent.AddImpulse` (`self.Item Mesh`) (* (+ ShotFromDirection (0.0 0.0 1.0)) 800.0) "None" true))

(event `self.Update Physics`
  (bind _audio (`self.Audio`))
  (`parent.Update Physics`)
  (`SceneComponent.SetVisibility` (`self.P_AOE_Trail_FireAndSmoke`) (`self.Physics Enabled`) false)
  (if (`self.Physics Enabled`)
    (`AudioComponent.Play` _audio 0.0)
    (else
      (`AudioComponent.Stop` _audio))))

(event `Start Rand Torque Timer`
  (bind _returnvalue (`KismetSystemLibrary.K2_SetTimerDelegate` (`|CreateDelegate` :!event `Rand Torque`) (`KismetMathLibrary.RandomFloatInRange` 0.3 0.6)))
  (set `self.Torque Timer` _returnvalue))

(event `Server Explode`
  (params (Location :type "Vector Structure"))
  (`/Engine/EditorBlueprintResources/StandardMacros.DoOnce` false
    (:`Completed`
      (set `self.Physics Enabled` false)
      (`KismetSystemLibrary.Delay` 0.02)
      (`self.MC Explode` (`self.K2_GetActorLocation`))
      (`GameplayStatics.ApplyRadialDamage` :`BaseDamage` (`self.Damage`) :`Origin` Location :`DamageRadius` (`self.Damage Radius`) :`DamageTypeClass` (`self.Explosive Damage Type Class`) :`DamageCauser` self :`InstigatedByController` null :`bDoFullDamage` true :`DamagePreventionChannel` "ECC_GameTraceChannel6")
      (set `RadialForceComponent.Radius` (`self.Damage Radius`) (`self.RadialForce`))
      (`RadialForceComponent.FireImpulse` (`self.RadialForce`))
      (`KismetSystemLibrary.Delay` 2.0)
      (`self.K2_DestroyActor`))))

(event `MC Explode`
  (params (Location :type "Vector Structure"))
  (`NiagaraFunctionLibrary.SpawnSystemAtLocation` (`self.Niagara`) Location)
  (`GameplayStatics.PlaySoundAtLocation` (`self.Explosive Sound`) Location (struct) 1.0 1.0 0.0 null null null null)
  (`self.SetActorHiddenInGame` true)
  (`self.SetActorEnableCollision` false))

(event `Set Can Fly`
  (`/Engine/EditorBlueprintResources/ActorMacros.Switch Has Authority`
    (:`Authority`
      (`self.Drop`)
      (set `self.Physics Enabled` true)
      (`TimelineComponent.PlayFromStart` (`self.gas force`))
      (`self.Rand Torque`)
      (`KismetSystemLibrary.Delay` (`self.Fly Time`))
      (`self.Server Explode` (`SceneComponent.K2_GetComponentLocation` (`self.Item Mesh`))))))

(event `Rand Torque`
  (set `self.Desired Rotation` (`KismetMathLibrary.RandomRotator` true))
  (`self.Start Rand Torque Timer`))

(event `self.ReceiveTick`
  (params (DeltaSeconds :type "Float (single-precision)"))
  (if (`self.Physics Enabled`)
    (`PrimitiveComponent.AddTorqueInDegrees` (`self.Item Mesh`) (* (`KismetMathLibrary.RandomUnitVector`) 5000.0) "None" true)))

(fn `UserConstructionScript`
  (`parent.UserConstructionScript`))