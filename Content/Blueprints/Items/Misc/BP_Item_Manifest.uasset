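; BP_Item_Manifest is the manifest item, a child Blueprint that adds small visual tweaks to its parent's equip behavior.
; On equip it calls the parent, then deactivates its RotatingMovement component.
; On unequip it calls the parent, then turns on custom depth rendering for ItemMesh.
; StopFocus is overridden empty with no parent call, so any inherited focus-loss behavior is skipped.
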(event `self.On Equipped`
  (params (NewOwner :type "Actor Object Reference"))
  (`parent.On Equipped` NewOwner)
  (`ActorComponent.Deactivate` (`self.RotatingMovement`)))

(event `self.On Unequipped`
  (`parent.On Unequipped`)
  (`PrimitiveComponent.SetRenderCustomDepth` (`self.Item Mesh`) true))

(event `/Game/Primer/Primer_Interaction/BPI_Interact.Stop Focus`)

(fn `UserConstructionScript`
  (`parent.UserConstructionScript`))