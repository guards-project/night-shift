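; Auto turret pawn that targets characters its team component allows within a range sphere and fires a child-actor ranged weapon at them.
; Sphere overlaps rebuild the target list and toggle a looping retarget timer.
; Firing evaluation picks the nearest target in line of sight, firing on authority only when the muzzle aligns with the weapon's suggested velocity.
; Tick turns yaw and pitch components toward that velocity; OnRep forwards target changes.
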(event `self.ReceiveBeginPlay`
  (`/Engine/EditorBlueprintResources/ActorMacros.Switch Has Authority`
    (:`Authority`
      (bind _asbp_item_ranged_weapon (cast `/Game/Blueprints/Items/Ranged/BP_Item_RangedWeapon` (`ChildActorComponent.ChildActor` (`self.Weapon`))))
      (set `self.Ref Ranged Weapon` _asbp_item_ranged_weapon))))

(event `self.Sphere.OnComponentBeginOverlap`
  (params (OverlappedComponent :type "PrimitiveComponent Object Reference") (OtherActor :type "Actor Object Reference") (OtherComp :type "PrimitiveComponent Object Reference") (OtherBodyIndex :type Integer) (bFromSweep :type Boolean) (SweepResult :type "HitResult Structure (by ref)"))
  (`self.Evaluate Targets` :!label _label))

(event `self.Sphere.OnComponentEndOverlap`
  (params (OverlappedComponent :type "PrimitiveComponent Object Reference") (OtherActor :type "Actor Object Reference") (OtherComp :type "PrimitiveComponent Object Reference") (OtherBodyIndex :type Integer))
  (goto _label))

(event `self.ReceiveTick`
  (params (DeltaSeconds :type "Float (single-precision)"))
  (`self.Update Rotations`))

(fn `Evaluate Firing`
  (bind (_world_transform_location _world_transform_rotation) (`KismetMathLibrary.BreakTransform` (`/Game/Blueprints/Items/Ranged/BP_Item_RangedWeapon.Get Muzzle` (`self.Ref Ranged Weapon`))))
  (`|ExecutionSequence`
    (:`then_0`
      (bind _target (`self.Get Best Target`))
      (`self.Set Target` _target))
    (:`then_1`
      (bind _target_2 (`self.Target`)
        (:`then`
          (bind (_can_fire _prediction_velocity) (`self.Get Can Fire` _target_2))
          (if _can_fire
            (`self.Set Firing` (> (`KismetMathLibrary.Dot_VectorVector` (`KismetMathLibrary.Normal` _prediction_velocity) (`KismetMathLibrary.Conv_RotatorToVector` _world_transform_rotation)) (`self.Firing Dot`)))
            (else
              (`self.Set Firing` false))))
        (:`else`)))))

(fn `Evaluate Targets`
  (`KismetArrayLibrary.Array_Clear` (`self.Targets in Range`))
  (for _array_element (`PrimitiveComponent.GetOverlappingActors` (`self.Sphere`) "/Game/Blueprints/Core/BP_Character_Template.BP_Character_Template_C")
    (bind _returnvalue (`self.GetComponentByClass` _array_element "/Game/Blueprints/Core/Components/BP_Team_Component.BP_Team_Component_C"))
    (`/Engine/EditorBlueprintResources/StandardMacros.IsValid` _returnvalue
      (:`Is Valid`
        (if (`/Game/Blueprints/Core/Components/BP_Team_Component.Can Target` (`self.BP_Team_Component`) _returnvalue)
          (`KismetArrayLibrary.Array_Add` (`self.Targets in Range`) _array_element)))))
  (`|ExecutionSequence`
    (:`then_0`
      ;[1 1 1] IF > had a target that left range
      ; THEN > clear target
      (if (not (`KismetArrayLibrary.Array_Contains` (`self.Targets in Range`) (`self.Target`)))
        (`self.Set Target` null)))
    (:`then_1`
      (if (`KismetArrayLibrary.Array_IsEmpty` (`self.Targets in Range`))
        ;[1 1 1] If there are no targets, stop retargetting
        (`KismetSystemLibrary.K2_ClearAndInvalidateTimerHandle` (`self.Retarget Handle`))
        (else
          ;[1 1 1] If there are targets, start retargetting logic unless already active
          (if (not (`KismetSystemLibrary.K2_IsTimerActiveHandle` (`self.Retarget Handle`)))
            (bind _returnvalue_2 (`KismetSystemLibrary.K2_SetTimerDelegate` (`|CreateDelegate` :!event `Evaluate Firing`) (`self.Retarget Interval`) true))
            (set `self.Retarget Handle` _returnvalue_2)))))))

(fn `Get Best Target`
  (returns (Target :type "Actor Object Reference"))
  (locals (`L Nearest` :type "Float (double-precision)" :default 99999.0) (`L Best Target` :type "Actor Object Reference"))
  (for _array_element (`self.Targets in Range`)
    (bind _can_fire (`self.Get Can Fire` _array_element))
    (if _can_fire
      (bind _returnvalue (`self.GetDistanceTo` _array_element self))
      (if (< _returnvalue (`local.L Nearest`))
        (set `local.L Nearest` _returnvalue)
        (set `local.L Best Target` _array_element))))
  (return (`local.L Best Target`)))

(fn `Get Can Fire`
  (params (Actor :type "Actor Object Reference"))
  (returns (`Can Fire` :type Boolean) (`Prediction Velocity` :type "Vector Structure"))
  (bind _returnvalue (`self.GetController`))
  (bind _ref_ranged_weapon (`self.Ref Ranged Weapon`)
    (:`then`
      (`/Engine/EditorBlueprintResources/StandardMacros.IsValid` _returnvalue
        (:`Is Valid`
          (bind _world_transform_location (`KismetMathLibrary.BreakTransform` (`/Game/Blueprints/Items/Ranged/BP_Item_RangedWeapon.Get Muzzle` _ref_ranged_weapon)))
          (bind _returnvalue_2 (`Controller.LineOfSightTo` _returnvalue (`local.Actor`) _world_transform_location false))
          (if _returnvalue_2
            (bind _prediction_velocity (`/Game/Blueprints/Items/Ranged/BP_Item_RangedWeapon.Suggest Velocity` _ref_ranged_weapon (`local.Actor`) -20.0))
            (return _returnvalue_2 _prediction_velocity)
            (else
              (return false (0.0 0.0 0.0)))))))
    (:`else`)))

(fn `On Gained Target`)

(fn `On Lost Target`
  (bind _target (`self.Get Best Target`))
  (`/Engine/EditorBlueprintResources/StandardMacros.IsValid` _target
    (:`Is Valid`
      (`self.Set Target` _target))))

(fn `On Target Changed`
  (params (Target :type "Actor Object Reference")))

(fn `OnRep_Target`
  (`self.On Target Changed` (`self.Target`)))

(fn `Set Firing`
  (params (Firing :type Boolean))
  (bind _ref_ranged_weapon (`self.Ref Ranged Weapon`))
  (`/Engine/EditorBlueprintResources/ActorMacros.Switch Has Authority`
    (:`Authority`
      (if Firing
        (`/Game/Blueprints/Items/Ranged/BP_Item_RangedWeapon.Start Firing` _ref_ranged_weapon)
        (else
          (`/Game/Blueprints/Items/Ranged/BP_Item_RangedWeapon.Stop Firing` _ref_ranged_weapon))))))

(fn `Set Target`
  (params (Target :type "Actor Object Reference"))
  (if (!= Target (`self.Target`))
    (bind _output_get (set `self.Target` Target))
    (`self.Set Firing` false)
    (`/Engine/EditorBlueprintResources/StandardMacros.IsValid` _output_get
      (:`Is Valid`
        ;[1 1 1] Comment
        (`self.On Gained Target`))
      (:`Is Not Valid`
        ;[1 1 1] Find another target
        (`self.On Lost Target`)))))

(fn `Update Rotations`
  (bind _returnvalue (`self.GetTransform`))
  (bind (_relativerotation_roll _relativerotation_pitch) (`KismetMathLibrary.BreakRotator` (`SceneComponent.RelativeRotation` (`self.Yaw`))))
  (bind (_relativerotation_roll_2 _relativerotation_pitch_2 _relativerotation_yaw) (`KismetMathLibrary.BreakRotator` (`SceneComponent.RelativeRotation` (`self.Pitch`))))
  (`self.Ref Ranged Weapon`
    (:`then`
      (bind _target (`self.Target`)
        (:`then`
          (bind (_can_fire _prediction_velocity) (`self.Get Can Fire` _target))
          (bind _returnvalue_2 (`KismetMathLibrary.Normal` _prediction_velocity))
          (bind (_returnvalue_roll _returnvalue_pitch _returnvalue_yaw) (`KismetMathLibrary.BreakRotator` (`KismetMathLibrary.MakeRotFromX` (`KismetMathLibrary.InverseTransformDirection` _returnvalue _returnvalue_2))))
          (`SceneComponent.K2_SetRelativeRotation` (`self.Yaw`) (`KismetMathLibrary.MakeRotator` _relativerotation_roll _relativerotation_pitch _returnvalue_yaw) false false)
          (bind (_returnvalue_roll_2 _returnvalue_pitch_2) (`KismetMathLibrary.BreakRotator` (`KismetMathLibrary.Conv_VectorToRotator` (`KismetMathLibrary.InverseTransformDirection` _returnvalue _returnvalue_2))))
          (`SceneComponent.K2_SetRelativeRotation` (`self.Pitch`) (`KismetMathLibrary.MakeRotator` _relativerotation_roll_2 _returnvalue_pitch_2 _relativerotation_yaw) false false))
        (:`else`)))
    (:`else`)))

(fn `UserConstructionScript`
  (`SphereComponent.SetSphereRadius` (`self.Sphere`) (`self.Range`) true))