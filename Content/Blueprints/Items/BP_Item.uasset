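; Base replicated item actor that characters pick up, equip in a weapon or shield socket, drop, throw, or steal from behind.
; Inventory drives equip and unequip; a replicated PhysicsEnabled flag toggles between socket attachment and simulated physics.
; Thrown hits fire gameplay cues and, on authority, deal damage, stun or guard-stagger via GAS and emit AI noise.
; Custom-depth highlights, temporary interact lockout and a last-owner loot beam aid retrieval.
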(event `self.ReceiveBeginPlay`
  (`self.Update Physics`))

(event `/Game/Primer/Primer_Interaction/BPI_Interact.Execute Interact`
  (params (User :type "Controller Object Reference"))
  ;[1 1 1] Interact Pickup
  (`/Engine/EditorBlueprintResources/ActorMacros.Switch Has Authority`
    (:`Authority`
      (`|ExecutionSequence`
        (:`then_0`
          (`self.Drop`))
        (:`then_1`
          (`self.Pickup` User))))))

(event `On Equipped`
  (params (NewOwner :type "Actor Object Reference"))
  (bind _returnvalue (`self.K2_GetActorLocation`))
  ;[1 1 1] Equip Unequip - Called from Inventory OnRep_EquippedItem
  (`self.SetOwner` NewOwner)
  (set `self.Last Owner` (`self.GetOwner`)) ; update the last owner after setting it
  (`self.Set Last Owner Glow` false)
  (`self.Set Ignore Owner`)
  (`PrimitiveComponent.SetCollisionResponseToChannel` (`self.Item Mesh`) "ECC_Visibility" "ECR_Ignore")
  (`self.ItemEquip` self)
  (`|ExecutionSequence`
    (:`then_0`
      (`/Engine/EditorBlueprintResources/ActorMacros.Switch Has Authority`
        (:`Authority`
          (set `self.Physics Enabled` false))))
    (:`then_1`
      (`/Engine/EditorBlueprintResources/StandardMacros.Can Execute Cosmetic Events`
        (:`True`
          (`self.End Temp Disable Interact`)
          (`self.Set Mesh Highlight` false)
          (if (!= _returnvalue (0.0 0.0 0.0) :`ErrorTolerance` 150.0)
            (`GameplayStatics.PlaySoundAtLocation` (`self.Pickup Sound`) _returnvalue (struct) 1.0 1.0 0.0 null null null null)))))))

(event `Temp Disable Interact`
  ;[1 1 1] Disable Interact
  (set `self.Can Ever Interact` false)
  (bind _returnvalue (`KismetSystemLibrary.K2_SetTimerDelegate` (delegate `Show White Highlight`) 1.0))
  (set `self.Temp Disable Timer` _returnvalue))

(event `Show White Highlight`
  ;[1 1 1] Disable Interact
  (set `self.Can Ever Interact` true)
  (`/Engine/EditorBlueprintResources/StandardMacros.IsValid` (`self.GetOwner`)
    (:`Is Not Valid`
      (`self.Set Mesh Highlight` true))))

(event `On Unequipped`
  ;[1 1 1] Equip Unequip - Called from Inventory OnRep_EquippedItem
  (`self.Overlap Characters Temp`)
  (`self.SetOwner` null)
  (`self.K2_DetachFromActor` "KeepWorld" "KeepWorld" "KeepWorld")
  (`PrimitiveComponent.SetCollisionResponseToChannel` (`self.Item Mesh`) "ECC_Visibility" "ECR_Block")
  (`self.ItemUnequip` self)
  (`|ExecutionSequence`
    (:`then_0`
      (`/Engine/EditorBlueprintResources/ActorMacros.Switch Has Authority`
        (:`Authority`
          (set `self.Physics Enabled` true))))
    (:`then_1`
      (`/Engine/EditorBlueprintResources/StandardMacros.Can Execute Cosmetic Events`
        (:`True`
          (`self.Temp Disable Interact`)
          (`self.Set Mesh Highlight` true)
          (`self.Set Last Owner Glow` true))))))

(event `End Temp Disable Interact`
  ;[1 1 1] Disable Interact
  (`KismetSystemLibrary.K2_ClearAndInvalidateTimerHandle` (`self.Temp Disable Timer`))
  (set `self.Can Ever Interact` true)
  (`/Engine/EditorBlueprintResources/StandardMacros.IsValid` (`self.GetOwner`)
    (:`Is Not Valid`
      (`self.Set Mesh Highlight` true))))

(event `Delay Disasble Beam`
  ;[1 1 1] Equip Unequip - Called from Inventory OnRep_EquippedItem
  (`self.Set Last Owner Glow` false))

(event `Pickup`
  (params (Controller :type "Controller Object Reference"))
  ;[1 1 1] Pickup Drop
  (bind _can_pickup (`self.Can Pickup`))
  (if _can_pickup
    (`/Game/Blueprints/Items/BP_Inventory_Component.Equip Item` (`self.GetComponentByClass` (`Controller.K2_GetPawn` Controller) "/Game/Blueprints/Items/BP_Inventory_Component.BP_Inventory_Component_C") self)
    (`self.ItemPickup` self)))

(event `Drop`
  (bind _returnvalue (`self.GetOwner`))
  (bind _returnvalue_2 (`self.GetComponentByClass` _returnvalue "/Game/Blueprints/Items/BP_Inventory_Component.BP_Inventory_Component_C"))
  ;[1 1 1] Pickup Drop
  (`/Engine/EditorBlueprintResources/StandardMacros.IsValid` _returnvalue
    (:`Is Valid`
      (`/Engine/EditorBlueprintResources/StandardMacros.IsValid` _returnvalue_2
        (:`Is Valid`
          (`/Game/Blueprints/Items/BP_Inventory_Component.Drop Item` _returnvalue_2 self)
          (`self.ItemDrop` self))))))

(event `self.ReceiveHit`
  (params (MyComp :type "PrimitiveComponent Object Reference") (Other :type "Actor Object Reference") (OtherComp :type "PrimitiveComponent Object Reference") (bSelfMoved :type Boolean) (HitLocation :type "Vector Structure") (HitNormal :type "Vector Structure") (NormalImpulse :type "Vector Structure") (Hit :type "HitResult Structure (by ref)"))
  ;[1 1 1] Play effect if velocity is > threshold or thrown
  ; deal damage if thrown
  (if (!= Other (`self.Last Owner`))
    (`/Engine/EditorBlueprintResources/StandardMacros.DoOnce` false :!label _label
      (:`Completed`
        (`|ExecutionSequence`
          (:`then_0`
            (set `self.Last Hit` Hit)
            (if (`self.Can Apply Thrown Hit`)
              (`self.Execute Gameplay Thrown Hit Cue`)
              (if (`self.Thrown`)
                (set `self.Thrown` false)
                (`/Engine/EditorBlueprintResources/ActorMacros.Switch Has Authority`
                  (:`Authority`
                    (`self.Apply Thrown Damage`))))))
          (:`then_1`
            (`KismetSystemLibrary.Delay` 0.2)
            (goto _label :!via `Reset`)))))))

(event `Ignore Items Temp`
  (`PrimitiveComponent.SetCollisionResponseToChannel` (`self.Item Mesh`) "ECC_GameTraceChannel2" "ECR_Ignore")
  (`KismetSystemLibrary.Delay` 1.0)
  (`PrimitiveComponent.SetCollisionResponseToChannel` (`self.Item Mesh`) "ECC_GameTraceChannel2" "ECR_Block"))

(event `/Game/Primer/Primer_Interaction/BPI_Interact.Start Focus`
  ;[1 1 1] Focus
  (`self.Set Mesh Highlight` true))

(event `Overlap Characters Temp`
  (bind _item_mesh (`self.Item Mesh`))
  (`PrimitiveComponent.SetCollisionResponseToChannel` _item_mesh "ECC_GameTraceChannel1" "ECR_Overlap")
  (`KismetSystemLibrary.Delay` 0.1)
  (`PrimitiveComponent.SetCollisionResponseToChannel` _item_mesh "ECC_GameTraceChannel1" "ECR_Block"))

(event `/Game/Primer/Primer_Interaction/BPI_Interact.Stop Focus`
  ;[1 1 1] Focus
  (`self.Set Mesh Highlight` false))

(event `Throw Item`
  (params (Location :type "Vector Structure") (Impulse :type "Vector Structure") (Torque :type "Vector Structure" :default (0.0 5000.0 0.0)) (Thrown :type Boolean))
  ;[1 1 1] Called from GA_ThrowItem & overlap enemy
  (`self.Drop`)
  (`PrimitiveComponent.SetCollisionEnabled` (`self.Item Mesh`) "QueryAndPhysics")
  (`self.K2_SetActorLocation` Location false true) ; moving actor so it does not clip the character who threw it - leads to issue where you can throw though a wall
  (`|ExecutionSequence`
    (:`then_0`
      (`PrimitiveComponent.SetSimulatePhysics` (`self.Item Mesh`) true)
      (`PrimitiveComponent.AddImpulse` (`self.Item Mesh`) Impulse "None" true)
      (`PrimitiveComponent.AddTorqueInDegrees` (`self.Item Mesh`) Torque "None" true)
      (set `self.Thrown` Thrown) ; see ricochet (sometimes we don't want the next 'throw' to deal damage
    )
    (:`then_1`
      (`/Engine/EditorBlueprintResources/ActorMacros.Switch Has Authority`
        (:`Authority`
          (set `self.Physics Enabled` true) ; late joiner state
        )))))

(event `self.Item Mesh.OnComponentBeginOverlap`
  (params (OverlappedComponent :type "PrimitiveComponent Object Reference") (OtherActor :type "Actor Object Reference") (OtherComp :type "PrimitiveComponent Object Reference") (OtherBodyIndex :type Integer) (bFromSweep :type Boolean) (SweepResult :type "HitResult Structure (by ref)"))
  ;[1 1 1] deprecated
  (set `self.Last Hit` SweepResult)
  (if (!= OtherActor (`self.Last Owner`))
    (if (`|EnumInequality` (`PrimitiveComponent.GetCollisionObjectType` OtherComp) "ECC_GameTraceChannel5")
      (if (`self.Can Apply Thrown Hit`)
        (`self.Execute Gameplay Thrown Hit Cue`)
        (`/Engine/EditorBlueprintResources/ActorMacros.Switch Has Authority`
          (:`Authority`
            (`|ExecutionSequence`
              (:`then_0`
                (if (`self.Thrown`)
                  (`self.Apply Thrown Damage`)))
              (:`then_1`
                (`self.Ricochet`)))))))))

(event `Ricochet`
  ;[1 1 1] deprecated
  (`/Engine/EditorBlueprintResources/StandardMacros.IsValid` self
    (:`Is Valid`
      (`/Engine/EditorBlueprintResources/StandardMacros.IsValid` (`self.GetAttachParentActor`)
        (:`Is Not Valid`
          (`self.Throw Item` (`self.K2_GetActorLocation`) (* (`KismetMathLibrary.GetReflectionVector` (* (`KismetMathLibrary.Normal` (`self.GetVelocity`)) -1.0) (`.Normal` (`GameplayStatics.BreakHitResult` (`self.Last Hit`)))) (* (`KismetMathLibrary.VSize` (`self.GetVelocity`)) 1.5)) (0.0 50000.0 0.0)))))))

(fn `Apply Thrown Damage`
  (bind (_bblockinghit _binitialoverlap _time _distance _location _impactpoint _normal _impactnormal _physmat _hitactor) (`GameplayStatics.BreakHitResult` (`self.Last Hit`)))
  (bind (_bblockinghit_2 _binitialoverlap_2 _time_2 _distance_2 _location_2 _impactpoint_2 _normal_2 _impactnormal_2 _physmat_2 _hitactor_2) (`GameplayStatics.BreakHitResult` (`self.Last Hit`)))
  (bind _returnvalue (`AbilitySystemBlueprintLibrary.GetAbilitySystemComponent` _hitactor_2))
  (bind _returnvalue_2 (`AbilitySystemBlueprintLibrary.GetAbilitySystemComponent` _hitactor))
  (if (> (`self.Thrown Hit Damage`) 0.0)
    (if (!= (`.HitActor` (`GameplayStatics.BreakHitResult` (`self.Last Hit`))) (`self.Last Owner`))
      (`|ExecutionSequence`
        (:`then_0`
          ;[1 1 1] Damage
          (`self.Clear Character Constraints` _hitactor)
          (if (`GSCBlueprintFunctionLibrary.HasAnyMatchingGameplayTag` (`.HitActor` (`GameplayStatics.BreakHitResult` (`self.Last Hit`))) (struct :`GameplayTags` (struct :`(TagName` "State.Guarding") :`(TagName` "State.Shielding"))))
            (`/Engine/EditorBlueprintResources/StandardMacros.IsValid` _returnvalue_2
              (:`Is Valid`
                (`AbilitySystemComponent.BP_ApplyGameplayEffectToSelf` _returnvalue_2 "/Game/Blueprints/GAS/Effects/GE_GuardStagger.GE_GuardStagger_C" 0.0 (`AbilitySystemComponent.MakeEffectContext` _returnvalue_2))))
            (else
              (`GameplayStatics.ApplyPointDamage` _hitactor (`self.Thrown Hit Damage`) (`self.Get Thrown Hit Direction` (`self.Last Hit`)) (`self.Last Hit`) (`self.Get Damage Instigator`) self (`self.Thrown Hit Damage Type`)))))
        (:`then_1`
          ;[1 1 1] Apply Stun
          (if (not (`GSCBlueprintFunctionLibrary.HasAnyMatchingGameplayTag` _hitactor_2 (struct :`GameplayTags` (struct :`(TagName` "State.Guarding") :`(TagName` "State.Shielding")))))
            (`/Engine/EditorBlueprintResources/StandardMacros.IsValid` _returnvalue
              (:`Is Valid`
                (`AbilitySystemComponent.BP_ApplyGameplayEffectToSelf` _returnvalue (select `bool` (`self.ActorHasTag` _hitactor_2 "Player") :`false` "/Game/Blueprints/GAS/Effects/GE_Stun.GE_Stun_C" :`true` "/Game/Blueprints/GAS/Effects/GE_Stun_1s.GE_Stun_1s_C" :!type "GameplayEffect Class Reference") 0.0 (`AbilitySystemComponent.MakeEffectContext` _returnvalue))))))
        (:`then_2`
          ;[1 1 1] Hit Noise for AI
          (`/Game/Blueprints/Core/PolygonAI/SenseData/BPFL_Noise.Create Noise` self (+ (`self.K2_GetActorLocation`) (0.0 0.0 10.0)) (`self.Noise`)))))))

(fn `Can Apply Thrown Hit`
  (returns (ReturnValue :type Boolean))
  (return (`self.Thrown`)))

(fn `Can Pickup`
  (returns (`Can Pickup` :type Boolean))
  (return true))

(fn `Clear Character Constraints`
  (params (Object :type "Object Object Reference"))
  (bind _outactors (`KismetSystemLibrary.SphereOverlapActors` (`self.K2_GetActorLocation`) 50.0 (`|MakeArray` "ObjectTypeQuery7" "ObjectTypeQuery3" "ObjectTypeQuery4" :!type "EObjectTypeQuery Enum") "/Game/Blueprints/Core/BP_Character_Template.BP_Character_Template_C"))
  (for _array_element _outactors
    (bind _asbp_character_template (cast `/Game/Blueprints/Core/BP_Character_Template` _array_element))
    (for _array_element_2 (`/Game/Blueprints/Core/BP_Character_Template.Constraints` _asbp_character_template)
      (`/Engine/EditorBlueprintResources/StandardMacros.IsValid` _array_element_2
        (:`Is Valid`
          (`self.K2_DestroyActor` _array_element_2))))))

(fn `Create Hit Params`
  (params (SourceObject :type "Object Object Reference"))
  (returns (ReturnValue :type "GameplayCueParameters Structure"))
  (bind (_returnvalue_normalizedmagnitude _returnvalue_rawmagnitude _returnvalue_effectcontext _returnvalue_matchedtagname _returnvalue_originaltag _returnvalue_aggregatedsourcetags _returnvalue_aggregatedtargettags _returnvalue_location _returnvalue_normal _returnvalue_instigator _returnvalue_effectcauser _returnvalue_sourceobject _returnvalue_physicalmaterial _returnvalue_gameplayeffectlevel _returnvalue_abilitylevel _returnvalue_targetattachcomponent) (`AbilitySystemBlueprintLibrary.BreakGameplayCueParameters` (`GameplayCueFunctionLibrary.MakeGameplayCueParametersFromHitResult` (`self.Last Hit`))))
  ;[1 1 1] Cant set members on CueParams??
  (return (`AbilitySystemBlueprintLibrary.MakeGameplayCueParameters` _returnvalue_normalizedmagnitude _returnvalue_rawmagnitude _returnvalue_effectcontext _returnvalue_matchedtagname _returnvalue_originaltag _returnvalue_aggregatedsourcetags _returnvalue_aggregatedtargettags _returnvalue_location _returnvalue_normal _returnvalue_instigator self SourceObject _returnvalue_physicalmaterial _returnvalue_gameplayeffectlevel _returnvalue_abilitylevel _returnvalue_targetattachcomponent true)))

(fn `Execute Gameplay Thrown Hit Cue`
  (bind (_bblockinghit _binitialoverlap _time _distance _location _impactpoint _normal _impactnormal _physmat _hitactor) (`GameplayStatics.BreakHitResult` (`self.Last Hit`)))
  (`/Engine/EditorBlueprintResources/ActorMacros.Switch Has Authority`
    (:`Authority`
      (`GameplayCueFunctionLibrary.ExecuteGameplayCueOnActor` (select `bool` (`KismetSystemLibrary.IsValid` (`AbilitySystemBlueprintLibrary.GetAbilitySystemComponent` _hitactor)) :`false` (`self.Last Owner`) :`true` _hitactor) (`self.Get Hit Cue`) (`self.Create Hit Params` _hitactor)))))

(fn `Get Always Show Widget`
  (returns (`Always Show` :type Boolean))
  (return false))

(fn `Get Can Interact`
  (returns (ReturnValue :type Boolean))
  (bind _returnvalue (`self.GetOwner`))
  (bind _returnvalue_2 (`Controller.K2_GetPawn` (`GameplayStatics.GetPlayerController` 0)))
  ;[1 1 1] Allow interaction if not attached to anything (such as character, or a wall panel)
  ; Deny interaction if attached to local player (so players can steal enemy stuff / disarm)
  (if (`self.Can Ever Interact`)
    (`/Engine/EditorBlueprintResources/StandardMacros.IsValid` _returnvalue
      (:`Is Valid`
        (bind _ascharacter (cast `Character` _returnvalue)
          (:`then`
            (bind _dead (message `/Game/Blueprints/Core/BPI_Character.Is Dead` _ascharacter))
            (bind _ko (message `/Game/Blueprints/Core/BPI_Character.Is KO` _ascharacter))
            (if (or _ko _dead)
              (return true)
              (else
                (bind _returnvalue_3 (`Pawn.GetController` _ascharacter))
                (`/Engine/EditorBlueprintResources/StandardMacros.IsValid` _returnvalue_3
                  (:`Is Valid`
                    (if (`Controller.IsLocalPlayerController` _returnvalue_3)
                      (return false) ; cannot grab your own item
                      (else
                        _)))
                  (:`Is Not Valid`
                    _))
                (`/Engine/EditorBlueprintResources/StandardMacros.IsValid` _returnvalue_2
                  (:`Is Valid`
                    (return (>= (`KismetMathLibrary.Dot_VectorVector` (`self.GetActorForwardVector` _returnvalue_2) (`self.GetActorForwardVector` (`self.GetOwner`))) 0.3)) ; only steal if behind
                  )))))
          (:`CastFailed`
            _)))
      (:`Is Not Valid`
        _))
    (return true)
    (else
      (return false))))

(fn `Get Damage Instigator`
  (returns (ReturnValue :type "Controller Object Reference"))
  (bind _last_owner (`self.Last Owner`)
    (:`then`
      (return (`self.GetInstigatorController` _last_owner)))
    (:`else`
      (return null))))

(fn `Get Highlight Meshes`
  (returns (Meshes :type "Array of PrimitiveComponent Object Reference"))
  (return (`|MakeArray` (`self.Item Mesh`) :!type "PrimitiveComponent Object Reference")))

(fn `Get Hit Cue`
  (returns (`Gameplay Cue Tag Throw Hit` :type "GameplayTag Structure"))
  (bind (_bblockinghit _binitialoverlap _time _distance _location _impactpoint _normal _impactnormal _physmat _hitactor) (`GameplayStatics.BreakHitResult` (`self.Last Hit`)))
  (return (select `bool` (`GSCBlueprintFunctionLibrary.HasMatchingGameplayTag` _hitactor (struct :`TagName` "State.Shielding")) :`false` (select `bool` (`GSCBlueprintFunctionLibrary.HasMatchingGameplayTag` _hitactor (struct :`TagName` "State.Guarding")) :`false` (`self.Gameplay Cue Tag Throw Hit`) :`true` (struct :`TagName` "GameplayCue.Hit.Guarded")) :`true` (struct :`TagName` "GameplayCue.Hit.Shielded"))))

(fn `Get Interact Distance`
  (returns (Distance :type "Float (double-precision)"))
  (return 250.0))

(fn `Get Interact Duration`
  (returns (Duration :type "Float (double-precision)"))
  (return 0.0))

(fn `Get Interact Text`
  (returns (Text :type Text))
  (return (`self.Interact Text`)))

(fn `Get Interact Widget Class`
  (returns (`Widget Class` :type "/Game/Primer/Primer_Interaction/UI/W_Interact_Master Soft Class Reference"))
  (return (`self.Interact Widget`)))

(fn `Get Thrown Hit Direction`
  (params (Hit :type "HitResult Structure"))
  (returns (Direction :type "Vector Structure"))
  (bind _last_owner (`self.Last Owner`)
    (:`then`
      (return (`KismetMathLibrary.GetDirectionUnitVector` (`self.K2_GetActorLocation` _last_owner) (`self.K2_GetActorLocation`))))
    (:`else`
      (return (`.ImpactNormal` (`GameplayStatics.BreakHitResult` Hit))))))

(fn `Is Locally Equipped`
  (returns (ReturnValue :type Boolean))
  (bind _returnvalue (`self.GetOwner`))
  (`/Engine/EditorBlueprintResources/StandardMacros.IsValid` _returnvalue
    (:`Is Valid`
      (bind _ascharacter (cast `Character` _returnvalue)
        (:`then`
          (return (`Pawn.IsLocallyControlled` _ascharacter)))
        (:`CastFailed`
          _)))
    (:`Is Not Valid`
      _))
  (return false))

(fn `Make Cue Params`
  (params (HitResult :type "HitResult Structure (by ref)"))
  (returns (ReturnValue :type "GameplayCueParameters Structure"))
  (bind (_returnvalue_normalizedmagnitude _returnvalue_rawmagnitude _returnvalue_effectcontext _returnvalue_matchedtagname _returnvalue_originaltag _returnvalue_aggregatedsourcetags _returnvalue_aggregatedtargettags _returnvalue_location _returnvalue_normal _returnvalue_instigator _returnvalue_effectcauser _returnvalue_sourceobject _returnvalue_physicalmaterial _returnvalue_gameplayeffectlevel _returnvalue_abilitylevel _returnvalue_targetattachcomponent) (`AbilitySystemBlueprintLibrary.BreakGameplayCueParameters` (`GameplayCueFunctionLibrary.MakeGameplayCueParametersFromHitResult` HitResult)))
  (return (`AbilitySystemBlueprintLibrary.MakeGameplayCueParameters` _returnvalue_normalizedmagnitude _returnvalue_rawmagnitude _returnvalue_effectcontext _returnvalue_matchedtagname _returnvalue_originaltag _returnvalue_aggregatedsourcetags _returnvalue_aggregatedtargettags _returnvalue_location _returnvalue_normal _returnvalue_instigator _returnvalue_effectcauser (`.HitActor` (`GameplayStatics.BreakHitResult` (`local.HitResult`))) _returnvalue_physicalmaterial _returnvalue_gameplayeffectlevel _returnvalue_abilitylevel _returnvalue_targetattachcomponent true)))

(fn `OnRep_Physics Enabled`
  (`self.Update Physics`))

(fn `Set Ignore Owner`
  (bind _last_owner (`self.Last Owner`)
    (:`then`
      (`PrimitiveComponent.IgnoreActorWhenMoving` (`self.Item Mesh`) _last_owner true)
      (bind _ascharacter (cast `Character` _last_owner))
      (`PrimitiveComponent.IgnoreActorWhenMoving` (`Character.CapsuleComponent` _ascharacter) self true)
      (`PrimitiveComponent.IgnoreActorWhenMoving` (`Character.Mesh` _ascharacter) self true))
    (:`else`)))

(fn `Set Last Owner Glow`
  (params (Glow :type Boolean))
  (bind _returnvalue (`GameplayStatics.GetPlayerController` 0))
  (bind _returnvalue_2 (`Controller.K2_GetPawn` _returnvalue))
  (if Glow
    (`/Engine/EditorBlueprintResources/StandardMacros.IsValid` _returnvalue
      (:`Is Valid`
        (`/Engine/EditorBlueprintResources/StandardMacros.IsValid` _returnvalue_2
          (:`Is Valid`
            (if (== (`self.Last Owner`) _returnvalue_2)
              (bind _lootbeam (`self.LootBeam`)
                (:`then`
                  (`SceneComponent.SetHiddenInGame` _lootbeam false false)
                  (bind _returnvalue_3 (`KismetSystemLibrary.K2_SetTimerDelegate` (`|CreateDelegate` :!event `Delay Disasble Beam`) 60.0))
                  (set `self.Glow Beam Removal Handle` _returnvalue_3))
                (:`else`)))))))
    (else
      (`SceneComponent.SetHiddenInGame` (`self.LootBeam`) true false))))

(fn `Set Mesh Highlight`
  (params (Show :type Boolean))
  (for _array_element (`self.Get Highlight Meshes`)
    (`/Engine/EditorBlueprintResources/StandardMacros.IsValid` _array_element
      (:`Is Valid`
        (`PrimitiveComponent.SetRenderCustomDepth` _array_element (and (or Show (and (not (`KismetSystemLibrary.IsValid` (`self.GetOwner`))) (`self.White Fill Enabled`))) (`self.Can Ever Interact`)))))))

(fn `Set White Fill`
  (params (`White Fill Enabled` :type Boolean))
  (bind _item_mesh (`self.Item Mesh`))
  (set `self.White Fill Enabled` `White Fill Enabled`)
  (`PrimitiveComponent.SetCustomDepthStencilValue` _item_mesh (`KismetMathLibrary.SelectInt` 2 1 (`self.White Fill Enabled`)))
  (`PrimitiveComponent.SetRenderCustomDepth` _item_mesh (`self.White Fill Enabled`)))

(fn `Update Interact Bounds`
  (bind _interactbox (`self.InteractBox`))
  (bind (_returnvalue_origin _returnvalue_boxextent) (`KismetMathLibrary.BreakBoxSphereBounds` (`StaticMesh.GetBounds` (`StaticMeshComponent.StaticMesh` (`self.Item Mesh`)))))
  (`BoxComponent.SetBoxExtent` _interactbox (* _returnvalue_boxextent (`self.Interact Bounds Scale`)) true)
  (`SceneComponent.K2_SetRelativeLocation` _interactbox (+ (`KismetMathLibrary.InverseTransformLocation` (`self.GetTransform`) (`KismetSystemLibrary.GetComponentBounds` (`self.Item Mesh`))) (`self.Interact Bounds Offset`)) false false))

(fn `Update Loot Beam Location`
  (bind _returnvalue_origin (`KismetMathLibrary.BreakBoxSphereBounds` (`StaticMesh.GetBounds` (`StaticMeshComponent.StaticMesh` (`self.Item Mesh`)))))
  (`SceneComponent.K2_SetRelativeLocation` (`self.LootBeam`) _returnvalue_origin false false))

(fn `Update Physics`
  (`self.Item Mesh`
    (:`then`
      (if (`self.Physics Enabled`)
        (`PrimitiveComponent.SetCollisionEnabled` (`self.Item Mesh`) "QueryAndPhysics")
        (`self.Ignore Items Temp`)
        (bind _item_mesh (`self.Item Mesh`)
          (:`then`
            (`PrimitiveComponent.SetSimulatePhysics` _item_mesh true))
          (:`else`))
        (else
          (`PrimitiveComponent.SetSimulatePhysics` (`self.Item Mesh`) false)
          (`PrimitiveComponent.SetCollisionEnabled` (`self.Item Mesh`) (`self.Idle Collision`))
          (bind _asbp_character_template (cast `/Game/Blueprints/Core/BP_Character_Template` (`self.GetOwner`)))
          (bind _returnvalue (select `bool` (`|EnumEquality` (`self.Item Type`) "NewEnumerator1") :`false` (`/Game/Blueprints/Core/BP_Character_Template.WeaponSocket` _asbp_character_template) :`true` (`/Game/Blueprints/Core/BP_Character_Template.ShieldSocket` _asbp_character_template)))
          (set `SpringArmComponent.CameraRotationLagSpeed` (`self.Socket Rotation lag`) _returnvalue)
          (`self.K2_AttachToComponent` _returnvalue "None" "SnapToTarget" "SnapToTarget" "KeepWorld")
          (`self.K2_SetActorRelativeTransform` (`self.Relative Attach Transform`)))))
    (:`else`)))

(fn `UserConstructionScript`
  (`self.Update Interact Bounds`)
  (`self.Update Physics`)
  (`self.Update Loot Beam Location`))