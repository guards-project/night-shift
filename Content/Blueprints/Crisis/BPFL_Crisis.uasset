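; Blueprint function library for the Crisis system, giving access to the crisis and crisis ability components that live on the GameState.
; Lookups search the crisis components by slot or district ID, with an empty slot resolving to the selected district, and also expose that component's save data.
; Selection sets each component's selected flag by district ID match.
; The bind helper subscribes to every component's selection event and returns the currently selected one.
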(fn `Bind to Crisis Selected`
  (params (Event :type "Delegate (by ref)"))
  (returns (Selected :type "/Game/Blueprints/Crisis/BP_Crisis_Component Object Reference"))
  (bind _returnvalue (`self.Get Crisis Components` null))
  (add `/Game/Blueprints/Crisis/BP_Crisis_Component.On District Selected` _returnvalue Event)
  (for _array_element _returnvalue
    (if (`/Game/Blueprints/Crisis/BP_Crisis_Component.District Selected` _array_element)
      (return _array_element))))

(fn `Get Crisis Ability Component`
  (returns (ReturnValue :type "/Game/_Guards/UserInterface/WorldMap/Crisis/BP_CrisisAbility_Component Object Reference"))
  (bind _returnvalue (`GameplayStatics.GetGameState` null))
  (`/Engine/EditorBlueprintResources/StandardMacros.IsValid` _returnvalue
    (:`Is Valid`
      (return (`Actor.GetComponentByClass` _returnvalue "/Game/_Guards/UserInterface/WorldMap/Crisis/BP_CrisisAbility_Component.BP_CrisisAbility_Component_C")))
    (:`Is Not Valid`
      (return null))))

(fn `Get Crisis Component`
  (params (Slot :type String))
  (returns (ReturnValue :type "/Game/Blueprints/Crisis/BP_Crisis_Component Object Reference"))
  (bind _returnvalue (`self.Get Crisis Components` null))
  (for _array_element _returnvalue
    (`/Engine/EditorBlueprintResources/StandardMacros.IsValid` _array_element
      (:`Is Valid`
        (if (or (`KismetStringLibrary.EqualEqual_StrStr` (`/Game/Blueprints/Crisis/BP_Crisis_Component.Slot` _array_element) (`KismetStringLibrary.Replace` (`local.Slot`) " ")) (and (`/Game/Blueprints/Crisis/BP_Crisis_Component.District Selected` _array_element) (`KismetStringLibrary.IsEmpty` (`local.Slot`))))
          (return _array_element)))))
  (return null))

(fn `Get Crisis Component by District ID`
  (params (ID :type Byte))
  (returns (ReturnValue :type "/Game/Blueprints/Crisis/BP_Crisis_Component Object Reference"))
  (bind _returnvalue (`self.Get Crisis Components` null))
  (for _array_element _returnvalue
    (if (== (`/Game/Blueprints/Crisis/BP_Crisis_Component.District ID` _array_element) ID)
      (return _array_element)))
  (return null))

(fn `Get Crisis Components`
  (returns (ReturnValue :type "Array of /Game/Blueprints/Crisis/BP_Crisis_Component Object Reference"))
  (bind _returnvalue (`GameplayStatics.GetGameState` null))
  (`/Engine/EditorBlueprintResources/StandardMacros.IsValid` _returnvalue
    (:`Is Valid`
      (return (`Actor.K2_GetComponentsByClass` _returnvalue "/Game/Blueprints/Crisis/BP_Crisis_Component.BP_Crisis_Component_C")))
    (:`Is Not Valid`
      (return))))

(fn `Get Crisis Save Data`
  (params (Slot :type String))
  (returns (`Crisis Save` :type "/Game/Blueprints/Crisis/BP_SaveGame_Crisis Object Reference"))
  (bind _returnvalue (`self.Get Crisis Component` Slot))
  (`/Engine/EditorBlueprintResources/StandardMacros.IsValid` _returnvalue
    (:`Is Valid`
      (bind _crisis_save (`/Game/Blueprints/Crisis/BP_Crisis_Component.Get Crisis Save` _returnvalue))
      (return _crisis_save))
    (:`Is Not Valid`
      (return null))))

(fn `Server Set Selected District`
  (params (ID :type Byte))
  (locals (`L Comp` :type "/Game/Blueprints/Crisis/BP_Crisis_Component Object Reference"))
  (bind _returnvalue (`GameplayStatics.GetGameState` null))
  (`/Engine/EditorBlueprintResources/StandardMacros.IsValid` _returnvalue
    (:`Is Valid`
      (for _array_element (`Actor.K2_GetComponentsByClass` _returnvalue "/Game/Blueprints/Crisis/BP_Crisis_Component.BP_Crisis_Component_C")
        (set `local.L Comp` _array_element)
        (`/Game/Blueprints/Crisis/BP_Crisis_Component.Set Selected District` (`local.L Comp`) (== (`/Game/Blueprints/Crisis/BP_Crisis_Component.District ID` _array_element) (`local.ID`)))))))