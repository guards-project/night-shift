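; SaveGame object for Crisis mode, storing case ID, Intel and Doom totals, missions, selected mission and crisis state.
; Mission results add the selected mission's Intel on a win or Doom on a loss, changing the crisis state when that total reaches 8.
; Setters and progress updates save to the slot immediately and call a data-updated notification.
; ApplyData copies saved values into by-ref parameters and returns missions and state.
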(fn `Apply Data`
  (params (`Case ID` :type "String (by ref)") (Intel :type "Integer (by ref)") (Doom :type "Integer (by ref)") (`Selected Mission` :type "Integer (by ref)"))
  (returns (`Crisis Missions` :type "Array of /Game/Blueprints/Crisis/F_CrisisMission Structure") (`Crisis State` :type "/Game/Blueprints/Crisis/E_CrisisState Enum"))
  (`|VariableSetRef` `Case ID` (`self.Case ID`))
  (`|VariableSetRef` Intel (`self.Intel`))
  (`|VariableSetRef` Doom (`self.Doom`))
  (`|VariableSetRef` `Selected Mission` (`self.Selected Crisis Mission`))
  (return (`self.Crisis Missions`) (`self.Crisis State`)))

(fn `Apply Mission Progress`
  (params (Win :type Boolean))
  (bind (_intel _doom) (break `/Game/Blueprints/Crisis/F_CrisisMission` (`|GetArrayItem` (`self.Crisis Missions`) (`self.Selected Crisis Mission`))))
  (`|ExecutionSequence`
    (:`then_0`
      (if Win
        (bind _output_get (set `self.Intel` (+ _intel (`self.Intel`))))
        (if (>= _output_get 8)
          (set `self.Crisis State` "NewEnumerator2"))
        (else
          (bind _output_get_2 (set `self.Doom` (+ _doom (`self.Doom`))))
          (if (>= _output_get_2 8)
            (set `self.Crisis State` "NewEnumerator3")))))
    (:`then_1`
      (`self.Save`))))

(fn `Save`
  (`GameplayStatics.SaveGameToSlot` self (`self.Save Name`))
  (`self.Data Updated`))

(fn `Set Crisis Mission Data`
  (params (Index :type Integer) (Item :type "/Game/Blueprints/Crisis/F_CrisisMission Structure (by ref)"))
  (`KismetArrayLibrary.Array_Set` (`self.Crisis Missions`) Index Item true)
  (`self.Save`))

(fn `Set Crisis State`
  (params (`Crisis State` :type "/Game/Blueprints/Crisis/E_CrisisState Enum" :default "NewEnumerator0"))
  (set `self.Crisis State` `Crisis State`)
  (`self.Save`))

(fn `Set Selected Crisis Mission`
  (params (`Selected Mission` :type Integer))
  (set `self.Selected Crisis Mission` `Selected Mission`)
  (set `self.Crisis State` "NewEnumerator1")
  (`self.Save`))