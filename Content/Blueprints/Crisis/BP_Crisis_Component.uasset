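; Replicated component running one district's crisis campaign: timed random missions, Intel and Doom meters, and a coin-based unlock.
; The authority loads the per-slot crisis save and player save into replicated state, whose OnReps notify listeners.
; In HubWorld, the selected district's in-progress crisis ages unselected missions, turning timeouts into Doom and rerolls.
; A once-gated state update pushes outcome modals, retrying if needed, and starts a new crisis after failure or completion.
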(event `self.ReceiveBeginPlay`
  (`/Engine/EditorBlueprintResources/ActorComponentMacros.Switch Has Authority`
    (:`Authority`
      (`self.Load Crisis Save`))))

(event `Draw Doom Widget`
  (`KismetSystemLibrary.Delay` 0.5)
  (`self.Failed Widget`
    (:`then`
      (`PanelWidget.ClearChildren` (`/Game/_Guards/UserInterface/WorldMap/Crisis/W_CrisisMissionFailed.VerticalBoxMission` (`self.Failed Widget`)) :!label _label)
      (for _array_element (`self.TimedOutMissions`)
        (`/Game/_Guards/UserInterface/WorldMap/Crisis/W_CrisisMissionFailed.Add Timeout Mission` (`self.Failed Widget`) _array_element))
      (`/Game/_Guards/UserInterface/WorldMap/Crisis/W_CrisisMissionFailed.Set Failed` (`self.Failed Widget`) (`|EnumEquality` (`self.Crisis State`) "NewEnumerator3")))
    (:`else`
      (bind (_commonstack _stack_modal) (`/Game/_Guards/UserInterface/Menus/Stack/BPFL_CommonStack.Push Modal` "/Game/_Guards/UserInterface/WorldMap/Crisis/W_CrisisMissionFailed.W_CrisisMissionFailed_C"))
      (`/Engine/EditorBlueprintResources/StandardMacros.IsValid` _stack_modal
        (:`Is Valid`
          (`KismetSystemLibrary.Delay` 0.01)
          (bind _asw_crisis_mission_failed (cast `/Game/_Guards/UserInterface/WorldMap/Crisis/W_CrisisMissionFailed` (`CommonActivatableWidgetContainerBase.GetActiveWidget` _stack_modal)))
          (set `self.Failed Widget` _asw_crisis_mission_failed)
          (goto _label))
        (:`Is Not Valid`
          (`KismetSystemLibrary.K2_SetTimerDelegate` (`|CreateDelegate` :!event `Draw Doom Widget`) 0.1))))))

(event `Draw Max Intel Widget`
  (`KismetSystemLibrary.Delay` 0.5)
  (bind (_commonstack _stack_modal) (`/Game/_Guards/UserInterface/Menus/Stack/BPFL_CommonStack.Push Modal` "/Game/_Guards/UserInterface/WorldMap/Crisis/W_CrisisIntelMax.W_CrisisIntelMax_C"))
  (`/Engine/EditorBlueprintResources/StandardMacros.IsValid` _stack_modal
    (:`Is Not Valid`
      (`KismetSystemLibrary.K2_SetTimerDelegate` (delegate `Draw Max Intel Widget`) 0.1))))

(event `On Intel Max Widget Created`
  (params (`Active Widget` :type "CommonActivatableWidget Object Reference")))

(event `Draw Case Complete Widget`
  (`KismetSystemLibrary.Delay` 0.5)
  (bind (_commonstack _stack_modal) (`/Game/_Guards/UserInterface/Menus/Stack/BPFL_CommonStack.Push Modal` "/Game/_Guards/UserInterface/WorldMap/Crisis/W_CrisisComplete.W_CrisisComplete_C"))
  (`/Engine/EditorBlueprintResources/StandardMacros.IsValid` _stack_modal
    (:`Is Not Valid`
      (`KismetSystemLibrary.K2_SetTimerDelegate` (delegate `Draw Case Complete Widget`) 0.1))))

(event `On Case Complete Created`
  (params (`Active Widget` :type "CommonActivatableWidget Object Reference")))

(event `Draw Case Failed Widget`
  (`KismetSystemLibrary.Delay` 0.5)
  (bind (_commonstack _stack_modal) (`/Game/_Guards/UserInterface/Menus/Stack/BPFL_CommonStack.Push Modal` "/Game/_Guards/UserInterface/WorldMap/Crisis/W_CrisisFailed.W_CrisisFailed_C"))
  (`/Engine/EditorBlueprintResources/StandardMacros.IsValid` _stack_modal
    (:`Is Not Valid`
      (`KismetSystemLibrary.K2_SetTimerDelegate` (delegate `Draw Case Failed Widget`) 0.1))))

(event `On Case Failed Created`
  (params (`Active Widget` :type "CommonActivatableWidget Object Reference")))

(event `Update State`
  ;[1 1 1] once per run update to state
  (if (`self.District Selected`)
    (if (`|EnumInequality` (`self.Crisis State`) "NewEnumerator0")
      (`/Engine/EditorBlueprintResources/StandardMacros.DoOnce` false :!label _label_2 ; reset in OnRep_CrisisState.MaxDoom
        (:`Completed`
          (switch `/Game/Blueprints/Crisis/E_CrisisState` (`self.Crisis State`)
            (:`NewEnumerator1`
              (`self.Reset State Gate`) ; If the state was in progress, \nallow new states to trigger such as max doom
              (`self.Resolve Anarchy`))
            (:`NewEnumerator2`
              (`self.Draw Max Intel Widget`))
            (:`NewEnumerator3`
              (`self.Draw Doom Widget`)
              (`self.Start New Crisis`))
            (:`NewEnumerator4`
              (`self.Draw Case Failed Widget`)
              (`self.Start New Crisis`))
            (:`NewEnumerator5`
              (`self.Draw Case Complete Widget`)
              (`self.Start New Crisis`))))))))

(event `Reset State Gate`
  ;[1 1 1] once per run update to state
  (goto _label_2 :!via `Reset`))

(fn `Add Days To All Missions`
  (params (`Days to Add` :type Integer))
  (locals (`L Save` :type "/Game/Blueprints/Crisis/BP_SaveGame_Crisis Object Reference"))
  (for (_ _array_index) (`self.Missions`)
    (`self.Add Days To Mission` _array_index `Days to Add`)))

(fn `Add Days To Mission`
  (params (`Mission Index` :type Integer) (`Days to Add` :type Integer))
  (locals (`L Save` :type "/Game/Blueprints/Crisis/BP_SaveGame_Crisis Object Reference"))
  (bind _mission_index (`local.Mission Index`))
  (bind _l_save (`local.L Save`))
  (bind _crisis_save (`self.Get Crisis Save`))
  (set `local.L Save` _crisis_save)
  (bind _crisis_missions (`/Game/Blueprints/Crisis/BP_SaveGame_Crisis.Crisis Missions` _crisis_save))
  (if (`KismetArrayLibrary.Array_IsValidIndex` _crisis_missions _mission_index)
    (bind _returnvalue (`|Copy` (`|GetArrayItem` _crisis_missions _mission_index)))
    (bind _structout (setmembers `/Game/Blueprints/Crisis/F_CrisisMission` :`StructRef` _returnvalue :`Days Left` (+ (`.DaysLeft_15_5EFD27F747EEAA411B641CA13E075EE6` (break `/Game/Blueprints/Crisis/F_CrisisMission` _returnvalue)) (`local.Days to Add`))))
    (`KismetArrayLibrary.Array_Set` (`/Game/Blueprints/Crisis/BP_SaveGame_Crisis.Crisis Missions` _l_save) (`local.Mission Index`) _structout)
    (`/Game/Blueprints/Crisis/BP_SaveGame_Crisis.Save` _l_save)
    (set `self.Missions` (`/Game/Blueprints/Crisis/BP_SaveGame_Crisis.Crisis Missions` (`local.L Save`)))))

(fn `Apply Player Save Data`
  (params (Save :type "/Game/Blueprints/Core/PlayerSave/SaveGame_Player Object Reference"))
  (locals (`L Save` :type "/Game/Blueprints/Core/PlayerSave/SaveGame_Player Object Reference"))
  (bind _last_crisis_slot (`/Game/Blueprints/Core/PlayerSave/SaveGame_Player.Last Crisis Slot` (`local.Save`)))
  (if (`KismetStringLibrary.IsEmpty` _last_crisis_slot)
    (set `/Game/Blueprints/Core/PlayerSave/SaveGame_Player.Last Crisis Slot` (`self.Slot`) (`local.Save`))
    (set `self.District Selected` true)
    (else
      (set `self.District Selected` (`KismetStringLibrary.EqualEqual_StrStr` _last_crisis_slot (`self.Slot`)))))
  (if (not (`.ReturnValue` (`BlueprintMapLibrary.Map_Find` (`/Game/Blueprints/Core/PlayerSave/SaveGame_Player.District Required Coins` (`local.Save`)) (`self.District ID`))))
    (`BlueprintMapLibrary.Map_Add` (`/Game/Blueprints/Core/PlayerSave/SaveGame_Player.District Required Coins` (`local.Save`)) (`self.District ID`) (`self.Unlock Cost`)))
  (`/Game/Blueprints/Core/PlayerSave/SaveGame_Player.Save` (`local.Save`)))

(fn `Apply Save to Replicated Data`
  (bind (_crisis_missions _crisis_state) (`/Game/Blueprints/Crisis/BP_SaveGame_Crisis.Apply Data` (`self.Crisis Save Data`) (`self.Case ID`) (`self.Intel`) (`self.Doom`) (`self.Selected Mission`)))
  (set `self.Missions` _crisis_missions)
  (set `self.Crisis State` _crisis_state)
  (`self.Data Loaded` self))

(fn `Complete Selected Mission`
  (params (Win :type Boolean))
  (bind _crisis_save (`self.Get Crisis Save`))
  (`/Game/Blueprints/Crisis/BP_SaveGame_Crisis.Apply Mission Progress` _crisis_save (`local.Win`))
  (`/Game/Blueprints/Crisis/BP_SaveGame_Crisis.Set Crisis Mission Data` _crisis_save (`/Game/Blueprints/Crisis/BP_SaveGame_Crisis.Selected Crisis Mission` _crisis_save) (`self.Create Random Mission`))
  (if (== (`/Game/Blueprints/Crisis/BP_SaveGame_Crisis.Doom` _crisis_save) 8)
    _))

(fn `Create Random Mission`
  (returns (`Out CrisisMission` :type "/Game/Blueprints/Crisis/F_CrisisMission Structure"))
  (locals (`L Mission Type` :type "/Game/_Guards/UserInterface/WorldMap/E_MissionType Enum"))
  (bind _l_mission_type (`local.L Mission Type`))
  (bind _outitem (`KismetArrayLibrary.Array_Random` (`self.Crisis Balancing`)))
  (`|ExecutionSequence`
    (:`then_0`
      ;[1 1 1] Randomize Type
      (if (`KismetArrayLibrary.Array_IsValidIndex` (`self.Allowed Missions`))
        (set `local.L Mission Type` (`KismetArrayLibrary.Array_Random` (`self.Allowed Missions`)))
        (else
          (set `local.L Mission Type` (cast `/Game/_Guards/UserInterface/WorldMap/E_MissionType` (`KismetMathLibrary.Conv_IntToByte` (`KismetMathLibrary.RandomInteger` (enumcount `/Game/_Guards/UserInterface/WorldMap/E_MissionType`)))))))
      (set `local.L Mission Type` (select `bool` (`|EnumEquality` _l_mission_type "NewEnumerator10") :`false` _l_mission_type :`true` "NewEnumerator8")) ; replace training with hostages
    )
    (:`then_1`
      ;[1 1 1] Randomize Result
      (return (make `/Game/Blueprints/Crisis/F_CrisisMission` (`KismetMathLibrary.FTrunc` (`KismetMathLibrary.BreakVector2D` _outitem)) (`KismetMathLibrary.FTrunc` (`.Y` (`KismetMathLibrary.BreakVector2D` _outitem))) (`local.L Mission Type`) 3 (`KismetArrayLibrary.Array_Random` (`self.Arrestable Perps`)))))))

(fn `Edit Doom`
  (params (Delta :type Integer :default -2))
  (locals (`L Save` :type "/Game/Blueprints/Crisis/BP_SaveGame_Crisis Object Reference"))
  (bind _crisis_save (`self.Get Crisis Save`))
  (bind _output_get (set `local.L Save` _crisis_save))
  (bind _output_get_2 (set `self.Doom` (`KismetMathLibrary.Max` (+ (`/Game/Blueprints/Crisis/BP_SaveGame_Crisis.Doom` _output_get) (`local.Delta`)))))
  (set `/Game/Blueprints/Crisis/BP_SaveGame_Crisis.Doom` _output_get_2 (`local.L Save`))
  (`/Game/Blueprints/Crisis/BP_SaveGame_Crisis.Save` (`local.L Save`)))

(fn `Edit Required Coins`
  (params (Coins :type Integer))
  (`/Engine/EditorBlueprintResources/ActorComponentMacros.Switch Has Authority`
    (:`Authority`
      (set `self.Required Coins` (- (`self.Required Coins`) Coins))
      (bind _player_save (`/Game/Blueprints/Core/BPFL_Guards.Get Player Save`))
      (`/Game/Blueprints/Core/PlayerSave/SaveGame_Player.Edit District Cost` _player_save (`self.District ID`) Coins))))

(fn `Get Crisis Save`
  (returns (`Crisis Save` :type "/Game/Blueprints/Crisis/BP_SaveGame_Crisis Object Reference"))
  (bind _slot (`self.Slot`))
  (bind _returnvalue (`GameplayStatics.DoesSaveGameExist` _slot))
  (if _returnvalue
    (bind _returnvalue_2 (`GameplayStatics.LoadGameFromSlot` _slot))
    (bind _asbp_save_game_crisis (cast `/Game/Blueprints/Crisis/BP_SaveGame_Crisis` _returnvalue_2))
    (set `self.Crisis Save Data` _asbp_save_game_crisis)
    (else
      (`self.Start New Crisis`)))
  (return (`self.Crisis Save Data`)))

(fn `Get Extract Mission Title`
  (params (`Perp Row` :type "DataTableRowHandle Structure (by ref)"))
  (returns (Result :type Text))
  (return "Objective_ExtractPerps"))

(fn `Get Mission Title`
  (returns (ReturnValue :type Text))
  (if (`|EnumEquality` (`.Mission_9_D1678DE44A2732A6D229299EAC24DA31` (break `/Game/Blueprints/Crisis/F_CrisisMission` (`self.Get Selected Mission`))) "NewEnumerator11")
    (bind _result (`self.Get Extract Mission Title` (`.ArrestPerp_18_BCA9C64F432D4B49948246B8787935B9` (break `/Game/Blueprints/Crisis/F_CrisisMission` (`self.Get Selected Mission`)))))
    (return _result)
    (else
      (return (`KismetTextLibrary.Conv_StringToText` (`|GetEnumeratorNameAsString` (`.Mission_9_D1678DE44A2732A6D229299EAC24DA31` (break `/Game/Blueprints/Crisis/F_CrisisMission` (`self.Get Selected Mission`)))))))))

(fn `Get Selected Mission`
  (returns (Output :type "/Game/Blueprints/Crisis/F_CrisisMission Structure (by ref)"))
  (return (make `/Game/Blueprints/Crisis/F_CrisisMission` 0 0 "NewEnumerator3")))

(fn `Is Locked`
  (returns (ReturnValue :type Boolean))
  (return (> (`self.Required Coins`) 0)))

(fn `Load Crisis Save`
  (bind _player_save (`/Game/Blueprints/Core/BPFL_Guards.Get Player Save`))
  (`/Engine/EditorBlueprintResources/StandardMacros.IsValid` _player_save
    (:`Is Valid`
      (`self.Apply Player Save Data` _player_save)
      (set `self.Required Coins` (`BlueprintMapLibrary.Map_Find` (`/Game/Blueprints/Core/PlayerSave/SaveGame_Player.District Required Coins` _player_save) (`self.District ID`)))
      (`self.Get Crisis Save`)
      (`self.Crisis Save Data`
        (:`then`
          (`KismetSystemLibrary.PrintString` "CRISIS: APPLY CRISIS DATA FROM SAVE" true true (struct :`G` 1.0 :`B` 0.110761 :`A` 1.0))
          (`self.Apply Save to Replicated Data`))
        (:`else`
          (`KismetSystemLibrary.PrintString` "ERROR: CRISIS SAVE FAILED TO LOAD" true true (struct :`R` 0.8125 :`G` 0.021159 :`B` 0.021159 :`A` 1.0)))))
    (:`Is Not Valid`
      (`KismetSystemLibrary.K2_SetTimerDelegate` (`|CreateDelegate` :!event `Load Crisis Save`) 0.2))))

(fn `OnRep_Crisis State`
  (`self.Update State`))

(fn `OnRep_District Selected`
  (`self.Data Loaded` self)
  (if (`self.District Selected`)
    (`self.On District Selected` self)
    (`self.Update State`)))

(fn `OnRep_Doom`
  (`self.Data Loaded` self))

(fn `OnRep_Missions`
  (`self.Data Loaded` self))

(fn `OnRep_Required Coins`
  (`self.District Coins Updated` self (`self.Required Coins`)))

(fn `OnRep_Selected Mission`
  (`self.Data Loaded` self))

(fn `OnRep_TimedOutMissions`
  (`self.Draw Doom Widget`))

(fn `Reroll Mission`
  (params (Index :type Integer))
  (bind _crisis_save (`self.Get Crisis Save`))
  (`/Game/Blueprints/Crisis/BP_SaveGame_Crisis.Set Crisis Mission Data` _crisis_save Index (`self.Create Random Mission`))
  (set `self.Missions` (`/Game/Blueprints/Crisis/BP_SaveGame_Crisis.Crisis Missions` _crisis_save)))

(fn `Resolve Anarchy`
  (locals (`L Mission` :type "/Game/Blueprints/Crisis/F_CrisisMission Structure") (`L Save` :type "/Game/Blueprints/Crisis/BP_SaveGame_Crisis Object Reference") (`L New Timeouts` :type "Array of /Game/Blueprints/Crisis/F_CrisisMission Structure") (`L Case Failed` :type Boolean))
  (bind _l_save (`local.L Save`))
  (bind _returnvalue (- (`.DaysLeft_15_5EFD27F747EEAA411B641CA13E075EE6` (break `/Game/Blueprints/Crisis/F_CrisisMission` (`local.L Mission`))) 1))
  (`/Engine/EditorBlueprintResources/ActorComponentMacros.Switch Has Authority`
    (:`Authority`
      (if (`self.District Selected`)
        (bind _returnvalue_2 (`GameplayStatics.GetCurrentLevelName` true))
        (if (`KismetStringLibrary.EqualEqual_StrStr` _returnvalue_2 "HubWorld")
          (if (`|EnumEquality` (`self.Crisis State`) "NewEnumerator1")
            ;[1 1 1] Tally Anarchy and draw toast in menu
            (bind _crisis_save (`self.Get Crisis Save`))
            (set `local.L Save` _crisis_save)
            (for (_array_element _array_index) (`/Game/Blueprints/Crisis/BP_SaveGame_Crisis.Crisis Missions` _crisis_save)
              (set `local.L Mission` _array_element)
              (if (!= _array_index (`/Game/Blueprints/Crisis/BP_SaveGame_Crisis.Selected Crisis Mission` _crisis_save))
                (if (<= _returnvalue 0)
                  (bind _output_get (set `self.Doom` (+ (`/Game/Blueprints/Crisis/BP_SaveGame_Crisis.Doom` (`local.L Save`)) (`.Doom_10_BFBF0A0342D78A1C09763C8453B5B002` (break `/Game/Blueprints/Crisis/F_CrisisMission` (`local.L Mission`))))))
                  (set `/Game/Blueprints/Crisis/BP_SaveGame_Crisis.Doom` _output_get (`local.L Save`))
                  (`KismetArrayLibrary.Array_Add` (`local.L New Timeouts`) (`local.L Mission`))
                  (set `local.L Mission` (`self.Create Random Mission`))
                  (`KismetArrayLibrary.Array_Set` (`/Game/Blueprints/Crisis/BP_SaveGame_Crisis.Crisis Missions` (`local.L Save`)) _array_index (`local.L Mission`))
                  (else
                    (setmembers `/Game/Blueprints/Crisis/F_CrisisMission` :`StructRef` (`local.L Mission`) :`Days Left` _returnvalue)
                    (`KismetArrayLibrary.Array_Set` (`/Game/Blueprints/Crisis/BP_SaveGame_Crisis.Crisis Missions` (`local.L Save`)) _array_index (`local.L Mission`))))))
            (set `self.Selected Mission` -1)
            (set `/Game/Blueprints/Crisis/BP_SaveGame_Crisis.Selected Crisis Mission` -1 _l_save)
            (`/Game/Blueprints/Crisis/BP_SaveGame_Crisis.Save` _l_save)
            (set `self.Missions` (`/Game/Blueprints/Crisis/BP_SaveGame_Crisis.Crisis Missions` _l_save))
            (`|ExecutionSequence`
              (:`then_0`
                (if (`KismetArrayLibrary.Array_IsValidIndex` (`local.L New Timeouts`))
                  (set `self.TimedOutMissions` (`local.L New Timeouts`))))
              (:`then_1`
                ;[1 1 1] Early Return if the case failed
                (if (>= (`self.Doom`) 8)
                  (set `self.Crisis State` "NewEnumerator3")
                  (return)
                  (else
                    (return)))))))))))

(fn `Set Selected District`
  (params (Selected :type Boolean))
  (`/Engine/EditorBlueprintResources/ActorComponentMacros.Switch Has Authority`
    (:`Authority`
      (if (!= Selected (`self.District Selected`))
        (bind _output_get (set `self.District Selected` Selected))
        (if _output_get
          (bind _player_save (`/Game/Blueprints/Core/BPFL_Guards.Get Player Save`))
          (set `/Game/Blueprints/Core/PlayerSave/SaveGame_Player.Last Crisis Slot` (`self.Slot`) _player_save)
          (`/Game/Blueprints/Core/PlayerSave/SaveGame_Player.Save` _player_save))))))

(fn `Start New Crisis`
  (locals (`L Missions` :type "Array of /Game/Blueprints/Crisis/F_CrisisMission Structure"))
  (`/Engine/EditorBlueprintResources/ActorComponentMacros.Switch Has Authority`
    (:`Authority`
      (`GameplayStatics.DeleteGameInSlot` (`self.Slot`))
      (bind _returnvalue (`GameplayStatics.CreateSaveGameObject` "/Game/Blueprints/Crisis/BP_SaveGame_Crisis.BP_SaveGame_Crisis_C"))
      (bind _output_get (set `self.Crisis Save Data` _returnvalue))
      ;[1 1 1] Multi district
      (set `/Game/Blueprints/Crisis/BP_SaveGame_Crisis.Save Name` (`self.Slot`) _output_get)
      ;[1 1 1] send state to save so that ApplySave()
      ; does not change state back to None (default).
      ;
      ; This fixes the issue where you complete or fail kingpin or have max doom, and the state is immediately reset upon calling StartNewCrisis()
      ;
      ; Clicking a mission at warmap_crisis will set state to InProgress which causes subsequent hub visits to increment days
      (set `/Game/Blueprints/Crisis/BP_SaveGame_Crisis.Crisis State` (`self.Crisis State`) _output_get)
      ;[1 1 1] Reset Doom
      (set `self.Doom` 0)
      (set `self.Intel` 0)
      ;[1 1 1] Set Random Case ID
      (set `/Game/Blueprints/Crisis/BP_SaveGame_Crisis.Case ID` (`KismetStringLibrary.Concat_StrStr` " #" (`KismetTextLibrary.Conv_TextToString` (`KismetTextLibrary.Conv_IntToText` (`KismetMathLibrary.RandomIntegerInRange` 1111 9999) false false))) (`self.Crisis Save Data`))
      ;[1 1 1] Create Random Missions
      (for _ (range (`self.Mission Option Count`))
        (`KismetArrayLibrary.Array_Add` (`local.L Missions`) (`self.Create Random Mission`)))
      (set `/Game/Blueprints/Crisis/BP_SaveGame_Crisis.Crisis Missions` (`local.L Missions`) (`self.Crisis Save Data`))
      (`GameplayStatics.SaveGameToSlot` (`self.Crisis Save Data`) (`self.Slot`))
      (`self.Apply Save to Replicated Data`))))