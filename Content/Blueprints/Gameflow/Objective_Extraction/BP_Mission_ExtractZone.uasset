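; Server-authoritative extraction zone that either ends a mission in victory or travels to a level.
; In extraction mode it is a singleton that activates when all registry missions complete, pointing to the Hub.
; Overlaps, pawn health events and joins/leaves recheck that every living, non-KO player is inside, then award arrest score and end the round.
; Otherwise, the host entering starts a short timer to load the target level, ignoring exits caused by seating.
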(event `self.ReceiveBeginPlay`
  (bind _returnvalue (`self.GetComponentByClass` (`GameplayStatics.GetGameMode`) "/Game/Blueprints/Core/Components/BP_PlayerJoinLeaveCallback.BP_PlayerJoinLeaveCallback_C"))
  ;[0 1 0.174] Init
  (`parent.ReceiveBeginPlay`)
  (`/Engine/EditorBlueprintResources/ActorMacros.Switch Has Authority`
    (:`Authority`
      (if (`self.Is Mission Extraction`)
        (`self.Singleton`)
        (`self.Bind to Last Mission Complete`)
        ;[1 1 1] Bind to players join/leave game to update the array of bound players for listening to pawn death
        (add `/Game/Blueprints/Core/Components/BP_PlayerJoinLeaveCallback.Player Joined` _returnvalue (`|CreateDelegate` :!event `On Player Joined or Left`))
        (add `/Game/Blueprints/Core/Components/BP_PlayerJoinLeaveCallback.Player Left` _returnvalue (`|CreateDelegate` :!event `On Player Joined or Left`))
        (`self.Bind to Player Pawn Events`)))))

(event `self.Sphere.OnComponentBeginOverlap`
  (params (OverlappedComponent :type "PrimitiveComponent Object Reference") (OtherActor :type "Actor Object Reference") (OtherComp :type "PrimitiveComponent Object Reference") (OtherBodyIndex :type Integer) (bFromSweep :type Boolean) (SweepResult :type "HitResult Structure (by ref)"))
  ;[1 1 1] Start and Stop Timer when Host Enters
  (`self.Check Overlap` OtherActor true))

(event `self.Sphere.OnComponentEndOverlap`
  (params (OverlappedComponent :type "PrimitiveComponent Object Reference") (OtherActor :type "Actor Object Reference") (OtherComp :type "PrimitiveComponent Object Reference") (OtherBodyIndex :type Integer))
  ;[1 1 1] Start and Stop Timer when Host Enters
  (`self.Check Overlap` OtherActor))

(event `Start Timer`
  ;[1 1 1] Start and Stop Timer when Host Enters
  (bind _returnvalue (`KismetSystemLibrary.K2_SetTimerDelegate` (delegate `Timer Complete`) 5.0))
  (set `self.Extract Timer` _returnvalue))

(event `Timer Complete`
  ;[1 1 1] Start and Stop Timer when Host Enters
  (`/Engine/EditorBlueprintResources/ActorMacros.Switch Has Authority`
    (:`Authority`
      (`self.Load Level`))))

(event `Stop Timer`
  ;[1 1 1] Start and Stop Timer when Host Enters
  (`KismetSystemLibrary.K2_ClearAndInvalidateTimerHandle` (`self.Extract Timer`)))

(event `Set Level Handle`
  (params (`World Handle` :type "DataTableRowHandle Structure"))
  ;[1 1 1] Load Level
  (set `self.World Handle` `World Handle`)
  (`self.Start Mission`))

(event `Load Level`
  ;[1 1 1] Load Level
  (set `self.Travelling` true)
  (bind _asbp_game_state_guards (cast `/Game/Blueprints/Core/BP_GameState_Guards` (`GameplayStatics.GetGameState`)))
  (`/Game/Blueprints/Core/BP_GameState_Guards.Go to Level` _asbp_game_state_guards (`KismetStringLibrary.Conv_StringToName` (`.LevelName_3_A4AFF82645491289FF83C88B1F78F9FF` (break `/Game/_Guards/UserInterface/WorldMap/F_World` (`self.Data`))))))

(event `self.Start Mission`
  (bind _sphere (`self.Sphere`))
  ;[1 1 1] Refresh
  (`parent.Start Mission`)
  (`PrimitiveComponent.SetCollisionEnabled` _sphere "NoCollision")
  (`PrimitiveComponent.SetCollisionEnabled` _sphere "QueryOnly"))

(event `On Pawn Destroyed`
  (params (DestroyedActor :type "Actor Object Reference"))
  ;[1 1 1] Wait for new pawn
  ; delay because new pawn will not
  ; immediately be ready after destruction
  (`KismetSystemLibrary.Delay` 0.2)
  (`self.Bind to Player Pawn Events`))

(event `Give Arrested Score`
  (`/Engine/EditorBlueprintResources/ActorMacros.Switch Has Authority`
    (:`Authority`
      (`/Engine/EditorBlueprintResources/StandardMacros.DoOnce` false
        (:`Completed`
          (set `self.Arrest Count` 0)
          (bind _returnvalue (`GameplayStatics.GetActorOfClass` "/Game/Blueprints/Gameflow/Objective_Extraction/BP_FollowerAutoStop.BP_FollowerAutoStop_C"))
          (`/Engine/EditorBlueprintResources/StandardMacros.IsValid` _returnvalue
            (:`Is Valid`
              (for _array_element (`GameStateBase.PlayerArray` (`GameplayStatics.GetGameState`))
                (`/Game/Blueprints/Core/Score/BPFL_Score.Add Score` (`PlayerState.GetPlayerName` _array_element) "Coins_Duty" (* (`KismetArrayLibrary.Array_Length` (`/Game/Blueprints/Gameflow/Objective_Extraction/BP_FollowerAutoStop.Cached` _returnvalue)) 20))))))))))

(fn `Bind to Last Mission Complete`
  (bind _returnvalue (`GameplayStatics.GetGameState`))
  (`/Engine/EditorBlueprintResources/StandardMacros.IsValid` _returnvalue
    (:`Is Valid`
      (bind _asbp_game_state_guards (cast `/Game/Blueprints/Core/BP_GameState_Guards` _returnvalue))
      (bind _output_get (set `self.Mission Registry` (`/Game/Blueprints/Core/BP_GameState_Guards.BP_MissionRegistry_Component_Guards` _asbp_game_state_guards)))
      (add `/Game/Primer/Primer_MissionHierarchy/BP_MissionRegistry_Component.All Missions Complete` _output_get (`|CreateDelegate` :!event `On All Missions Complete`))
      (bind _all_complete (`/Game/Primer/Primer_MissionHierarchy/BP_MissionRegistry_Component.Check All Missions Compete` _output_get))
      (if _all_complete
        (`self.On All Missions Complete` (`self.Mission Registry`))))
    (:`Is Not Valid`
      (`KismetSystemLibrary.K2_SetTimerDelegate` (`|CreateDelegate` :!event `Bind to Last Mission Complete`) 1.0))))

(fn `Bind to Player Pawn Events`
  (for _array_element (`GameStateBase.PlayerArray` (`GameplayStatics.GetGameState`))
    (bind _returnvalue (`PlayerState.GetPawn` _array_element))
    (`/Engine/EditorBlueprintResources/StandardMacros.IsValid` _returnvalue
      (:`Is Valid`
        ;[1 1 1] Bind to pawn death and recovery to recheck end condition
        ; because if a player dies in the field, all living player inside Extract Zone might succeed now
        (bind _asbp_character_template (cast `/Game/Blueprints/Core/BP_Character_Template` _returnvalue))
        ;;[1 1 1] todo convert to ENUM_HealthState or gameplay tag healthstate.dead,ko,etc?
        (add `/Game/Blueprints/Core/BP_Character_Template.OnDied` _asbp_character_template (`|CreateDelegate` :!event `On Pawn State Changed`))
        (add `/Game/Blueprints/Core/BP_Character_Template.OnKO` _asbp_character_template (`|CreateDelegate` :!event `On Pawn State Changed`))
        (add `/Game/Blueprints/Core/BP_Character_Template.OnRecovered` _asbp_character_template (`|CreateDelegate` :!event `On Pawn State Changed`))
        (add `/Game/Blueprints/Core/BP_Character_Template.OnRevived` _asbp_character_template (`|CreateDelegate` :!event `On Pawn State Changed`))
        ;[1 1 1] if the pawn was destroyed
        ; it may have left the map and respawned
        ; we should rebind to player pawns after this
        (add `self.OnDestroyed` _asbp_character_template (`|CreateDelegate` :!event `On Pawn Destroyed`)))
      (:`Is Not Valid`
        ;[1 1 1] pawn not valid, return early and try again
        ; can be due to dungeon generating and pausing pawn spawns
        (`KismetSystemLibrary.K2_SetTimerDelegate` (`|CreateDelegate` :!event `Bind to Player Pawn Events`) 0.2)
        (return))))
  (`self.Check End of Mission`))

(fn `Check End of Mission`
  (returns (Ended :type Boolean))
  (locals (`L Has Living Pawns` :type Boolean :default false))
  (if (and (`self.World is Valid`) (not (`self.Travelling`)))
    (bind _outactors (`GameplayStatics.GetAllActorsOfClass` "/Game/Blueprints/Core/BP_Character_Template_Player.BP_Character_Template_Player_C"))
    (for _array_element _outactors
      ;[1 1 1] Check for any living players outside the volume and return early - mission cannot end
      (bind _dead (message `/Game/Blueprints/Core/BPI_Character.Is Dead` _array_element))
      (bind _ko (message `/Game/Blueprints/Core/BPI_Character.Is KO` _array_element))
      (if (not (or _ko _dead))
        (if (`PrimitiveComponent.IsOverlappingActor` (`self.Sphere`) _array_element)
          (set `local.L Has Living Pawns` true)
          (else
            (return false) ; return fail
          ))))
    ;[1 1 1] if we didnt return early,
    ; then all living players are inside the extract zone
    (if (`local.L Has Living Pawns`)
      (`self.Give Arrested Score`)
      (bind _asbp_game_state_guards (cast `/Game/Blueprints/Core/BP_GameState_Guards` (`GameplayStatics.GetGameState`)))
      (`/Game/Blueprints/Core/BP_GameState_Guards.MC End Round` _asbp_game_state_guards true (`self.Get Context`) false)
      (return true) ; return success
    )))

(fn `Check Overlap`
  (params (Actor :type "Actor Object Reference") (Enter :type Boolean))
  (`/Engine/EditorBlueprintResources/ActorMacros.Switch Has Authority`
    (:`Authority`
      (if (and (`self.World is Valid`) (not (`self.Travelling`)))
        (if (`self.Is Mission Extraction`)
          (`self.Check End of Mission`)
          (else
            ;[1 1 1] APC Enter Exit (HOST ONLY)
            (bind _aspawn (cast `Pawn` (`local.Actor`)))
            (if (`Pawn.IsLocallyControlled` _aspawn)
              (if (`local.Enter`)
                (`self.Start Timer`)
                (else
                  (bind _asbp_character_template (cast `/Game/Blueprints/Core/BP_Character_Template` _aspawn))
                  (if (not (`/Game/Blueprints/Core/BP_Character_Template.Seated` _asbp_character_template))
                    (`self.Stop Timer`)))))))))))

(fn `Get Context`
  (returns (Context :type "Transform Structure"))
  (for _array_element (`GameStateBase.PlayerArray` (`GameplayStatics.GetGameState`))
    (bind _returnvalue (`PlayerState.GetPawn` _array_element))
    (`/Engine/EditorBlueprintResources/StandardMacros.IsValid` _returnvalue
      (:`Is Valid`
        (bind _dead (message `/Game/Blueprints/Core/BPI_Character.Is Dead` _returnvalue))
        (bind _ko (message `/Game/Blueprints/Core/BPI_Character.Is KO` _returnvalue))
        (if (not (or _ko _dead))
          (return (`self.GetTransform` _returnvalue))))))
  (return (`self.GetTransform`)))

(fn `Load World Data`
  (bind (_datatable _rowname) (break `DataTableRowHandle` (`self.World Handle`)))
  (bind _returnvalue (`|GetDataTableRow` _datatable _rowname)
    (:`then`
      (set `self.Data` _returnvalue))))

(fn `On All Missions Complete`
  (params (Registry :type "/Game/Primer/Primer_MissionHierarchy/BP_MissionRegistry_Component Object Reference"))
  (set `self.World Handle` (make `DataTableRowHandle` "/Game/_Guards/UserInterface/WorldMap/DT_HUBs.DT_HUBs" "Hub"))
  (`self.Start Mission`))

(fn `On Pawn State Changed`
  (params (Character :type "/Game/Blueprints/Core/BP_Character_Template Object Reference"))
  (`self.Check End of Mission`))

(fn `On Player Joined or Left`
  (params (Controller :type "Controller Object Reference") (PlayerState :type "PlayerState Object Reference"))
  (`self.Bind to Player Pawn Events`))

(fn `On World Handle Changed`
  (`self.Load World Data`)
  (`SceneComponent.SetHiddenInGame` (`self.Sphere`) (not (`self.World is Valid`)) false))

(fn `OnRep_World Handle`
  (`self.On World Handle Changed`)
  (`/Engine/EditorBlueprintResources/ActorMacros.Switch Has Authority`
    (:`Authority`
      (set `/Game/Primer/Primer_Markers/BP_Marker.Is Registered` (`self.World is Valid`) (`self.BP_Marker`)))))

(fn `Singleton`
  (bind _outactors (`GameplayStatics.GetAllActorsOfClass` "BP_Mission_ExtractZone_C"))
  (bind (_arrayindex _arrayelement) (`/Engine/EditorBlueprintResources/StandardMacros.ReverseForEachLoop` _outactors)
    (:`LoopBody`
      (if (!= _arrayelement self)
        (`self.K2_DestroyActor` _arrayelement)))))

(fn `UserConstructionScript`)

(fn `World is Valid`
  (returns (ReturnValue :type Boolean))
  (return (`KismetSystemLibrary.IsValid` (`.DataTable` (break `DataTableRowHandle` (`self.World Handle`))))))