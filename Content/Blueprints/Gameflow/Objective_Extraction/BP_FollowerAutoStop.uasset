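; Extraction objective trigger box that takes in following AI and assigns them a kneeling spot inside the mission's extraction zone.
; On the server, overlapping followers are tracked immediately, while other AI are watched for arrest and, if still inside with a player, set to follow that player and tracked.
; Tracking flags the AI, caches it, picks a random reachable point within the zone's sphere, and uncaches AI-tagged actors on death.
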(event `self.ReceiveBeginPlay`
  (bind _returnvalue (`GameplayStatics.GetActorOfClass` "/Game/Blueprints/Gameflow/Objective_Extraction/BP_Mission_ExtractZone.BP_Mission_ExtractZone_C"))
  (set `self.Extraction Zone` _returnvalue))

(event `self.Box.OnComponentBeginOverlap`
  (params (OverlappedComponent :type "PrimitiveComponent Object Reference") (OtherActor :type "Actor Object Reference") (OtherComp :type "PrimitiveComponent Object Reference") (OtherBodyIndex :type Integer) (bFromSweep :type Boolean) (SweepResult :type "HitResult Structure (by ref)"))
  (`self.Check Overlap` OtherActor))

(fn `BP_FollowerAutoStop_AutoGenFunc`
  (params (Character :type "/Game/Blueprints/Core/BP_Character_Template Object Reference") (Arrested :type Boolean))
  (bind _overlappingactors (`PrimitiveComponent.GetOverlappingActors` (`self.Box`) "/Game/Blueprints/Core/BP_Character_Template_Player.BP_Character_Template_Player_C"))
  (if Arrested
    (if (`PrimitiveComponent.IsOverlappingActor` (`self.Box`) Character)
      (bind _asbp_polygon_ai (cast `/Game/Blueprints/Core/PolygonAI/BP_Polygon_AI` Character))
      (if (`KismetArrayLibrary.Array_IsValidIndex` _overlappingactors)
        (`/Game/Blueprints/Core/PolygonAI/BP_Polygon_AI.Set Following` _asbp_polygon_ai (`Pawn.GetController` (cast `/Game/Blueprints/Core/BP_Character_Template_Player` (`|GetArrayItem` _overlappingactors) :!pure true)) true)
        (`self.Track Target` _asbp_polygon_ai)))))

(fn `Check Overlap`
  (params (Actor :type "Actor Object Reference"))
  (`/Engine/EditorBlueprintResources/ActorMacros.Switch Has Authority`
    (:`Authority`
      (bind _asbp_polygon_ai (cast `/Game/Blueprints/Core/PolygonAI/BP_Polygon_AI` Actor))
      (if (`/Game/Blueprints/Core/PolygonAI/BP_Polygon_AI.Following` _asbp_polygon_ai)
        (`self.Track Target` _asbp_polygon_ai)
        (else
          (add `/Game/Blueprints/Core/PolygonAI/BP_Polygon_AI.On Arrested Updated` _asbp_polygon_ai (`|CreateDelegate` :!event `BP_FollowerAutoStop_AutoGenFunc`)))))))

(fn `On Cached Enemy Died`
  (params (Character :type "/Game/Blueprints/Core/BP_Character_Template Object Reference"))
  (bind _asbp_polygon_ai (cast `/Game/Blueprints/Core/PolygonAI/BP_Polygon_AI` Character))
  (`KismetArrayLibrary.Array_RemoveItem` (`self.Cached`) _asbp_polygon_ai))

(fn `Track Target`
  (params (InputPin :type "/Game/Blueprints/Core/PolygonAI/BP_Polygon_AI Object Reference"))
  (bind _extraction_zone (`self.Extraction Zone`))
  (bind _inputpin (`local.InputPin`))
  (set `/Game/Blueprints/Core/PolygonAI/BP_Polygon_AI.At APC` true InputPin)
  (`KismetArrayLibrary.Array_AddUnique` (`self.Cached`) InputPin)
  (`|ExecutionSequence`
    (:`then_0`
      (bind _asai_controller_polygon (cast `/Game/Blueprints/Core/PolygonAI/Behaviour/AI_Controller_Polygon` (`AIBlueprintHelperLibrary.GetAIController` InputPin)))
      (`/Game/Blueprints/Core/PolygonAI/Behaviour/AI_Controller_Polygon.Set Kneeling Location` _asai_controller_polygon (`NavigationSystemV1.K2_GetRandomReachablePointInRadius` (`self.K2_GetActorLocation` _extraction_zone) (* (`.SphereRadius` (`KismetSystemLibrary.GetComponentBounds` (`/Game/Blueprints/Gameflow/Objective_Extraction/BP_Mission_ExtractZone.Sphere` _extraction_zone))) 0.8) null null)))
    (:`then_1`
      (if (`self.ActorHasTag` _inputpin "AI")
        (add `/Game/Blueprints/Core/BP_Character_Template.OnDied` _inputpin (`|CreateDelegate` :!event `On Cached Enemy Died`))))))

(fn `UserConstructionScript`)