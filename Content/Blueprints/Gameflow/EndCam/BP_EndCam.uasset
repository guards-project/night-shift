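; BP_EndCam is an end-of-game camera actor that plays a brief slow-motion swing shot when spawned.
; After a short delay for attachment death, it drops global time dilation, starts the camera, then restores normal speed.
; Where cosmetic events can execute, it becomes the first player's view target and a timeline swings the spring arm's yaw from side-on to zero.
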(event `self.ReceiveBeginPlay`
  (`KismetSystemLibrary.Delay` 0.2) ; allow attachment death to occur
  (`GameplayStatics.SetGlobalTimeDilation` 0.1)
  (`self.Play Cam`)
  (`KismetSystemLibrary.Delay` 0.35)
  (`GameplayStatics.SetGlobalTimeDilation` 1.0))

(event `Play Cam`
  (bind _springarm (`self.SpringArm`))
  (bind (_relativerotation_roll _relativerotation_pitch) (`KismetMathLibrary.BreakRotator` (`SceneComponent.RelativeRotation` _springarm)))
  (`/Engine/EditorBlueprintResources/StandardMacros.Can Execute Cosmetic Events`
    (:`True`
      (`PlayerController.SetViewTargetWithBlend` (`GameplayStatics.GetPlayerController` 0) self 0.0 "VTBlend_Linear" 0.0 true)
      (bind (_direction _newtrack_0) (`Timeline|CamTrack` :!via `PlayFromStart`)
        (:`Update`
          (`SceneComponent.K2_SetRelativeRotation` _springarm (`KismetMathLibrary.MakeRotator` _relativerotation_roll _relativerotation_pitch (`KismetMathLibrary.Lerp` 90.0 0.0 _newtrack_0)) false false))))))

(fn `UserConstructionScript`)