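; Hostage mission objective that completes once enough tracked hostages have been removed from play.
; After a short authority-only delay, it binds events on preset hostages and those overlapping its box, capping the target count by MaxTargets.
; Damage or removal can late-start the mission; destroyed hostages increment the count and trigger the state-gated win check.
; Timeout context uses a random remaining hostage's transform.
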(event `self.Start Mission`
  ;[1 1 1] Init mission, gather overlapping targets taking damage / death. start the mission if it isn't already started upon either event
  (`parent.Start Mission`)
  (`/Engine/EditorBlueprintResources/ActorMacros.Switch Has Authority`
    (:`Authority`
      (`KismetSystemLibrary.Delay` 0.2) ; This delay allows other actors to init\nso that box.overlappingactors works
      (`self.Track Overlapping Targets`) ; Tracking on begin play allows bindings to start the mission later if not already started
    )))

(event `On Enemy Died`
  (params (Character :type "/Game/Blueprints/Core/BP_Character_Template Object Reference"))
  ;[1 1 1] Target Tracking and Late Start Mission based on any events
)

(event `On Target Damaged`
  (params (DamagedActor :type "Actor Object Reference") (Damage :type "Float (single-precision)") (DamageType :type "DamageType Object Reference") (InstigatedBy :type "Controller Object Reference") (DamageCauser :type "Actor Object Reference"))
  ;[1 1 1] Target Tracking and Late Start Mission based on any events
  (`self.Handle Late Start Mission`))

(event `On Hostage Destroyed (saved)`
  (params (DestroyedActor :type "Actor Object Reference"))
  ;[1 1 1] Target Tracking and Late Start Mission based on any events
  (`self.Remove Target` DestroyedActor))

(fn `Add Target`
  (params (`New Target` :type "/Game/Blueprints/Core/PolygonAI/BP_Polygon_AI_Hostage Object Reference (by ref)"))
  (bind _new_target (`local.New Target`))
  (bind _returnvalue (`KismetArrayLibrary.Array_AddUnique` (`self.Hostages`) `New Target`))
  (`|ExecutionSequence`
    (:`then_0`
      (if (>= _returnvalue 0)
        (add `self.OnTakeAnyDamage` (`local.New Target`) (`|CreateDelegate` :!event `On Target Damaged`))
        (add `/Game/Blueprints/Core/BP_Character_Template.OnDied` _new_target (`|CreateDelegate` :!event `On Enemy Died`))
        (add `self.OnDestroyed` _new_target (`|CreateDelegate` :!event `On Hostage Destroyed (saved)`))
        (return)))
    (:`then_1`
      (return))))

(fn `Check Win`
  (returns (`Is Win` :type Boolean))
  (if (`|EnumEquality` (`self.Get Mission State`) "NewEnumerator3")
    (return (>= (`self.Current Count`) (`self.Target Count`)))
    (else
      (return false))))

(fn `Remove Target`
  (params (Actor :type "Actor Object Reference"))
  (bind _asbp_polygon_ai_hostage (cast `/Game/Blueprints/Core/PolygonAI/BP_Polygon_AI_Hostage` Actor))
  (bind _returnvalue (`KismetArrayLibrary.Array_RemoveItem` (`self.Hostages`) _asbp_polygon_ai_hostage))
  (if _returnvalue
    (set `self.Current Count` (+ (`self.Current Count`) 1))
    (`self.Handle Late Start Mission`)
    (bind _is_win (`self.Check Win`))
    (if _is_win
      (`self.Complete Mission` "NewEnumerator1"))))

(fn `Set Timeout Context`
  (set `self.Context` (`self.GetTransform` (`KismetArrayLibrary.Array_Random` (`self.Hostages`)))))

(fn `Track Overlapping Targets`
  (locals (`L Overlapped` :type "Array of Actor Object Reference"))
  (bind _max_targets (`self.Max Targets`))
  (bind _returnvalue (`KismetArrayLibrary.Array_Length` (`self.Hostages`)))
  ;[1 1 1] Track existing
  (for _array_element (`self.Hostages`)
    (`self.Add Target` _array_element))
  ;[1 1 1] Track Overlapping
  (for _array_element_2 (`PrimitiveComponent.GetOverlappingActors` (`self.Box`) "/Game/Blueprints/Core/PolygonAI/BP_Polygon_AI_Hostage.BP_Polygon_AI_Hostage_C")
    (bind _asbp_polygon_ai_hostage (cast `/Game/Blueprints/Core/PolygonAI/BP_Polygon_AI_Hostage` _array_element_2))
    (`self.Add Target` _asbp_polygon_ai_hostage))
  ;[1 1 1] Tally The Max Count
  (set `self.Target Count` (`KismetMathLibrary.Min` (`KismetMathLibrary.SelectInt` _max_targets _returnvalue (> _max_targets 0)) _returnvalue)))

(fn `UserConstructionScript`
  (`parent.UserConstructionScript`))