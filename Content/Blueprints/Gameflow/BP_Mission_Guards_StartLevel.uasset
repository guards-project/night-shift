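; BP_Mission_Guards_StartLevel is a gameflow mission objective that shows the player's next mission as its title.
; It binds to crisis selection and stores the crisis component whose district is selected.
; Each tick it builds a "NextMission: District - Mission" title from that component, substituting an arrest-chieftain objective in one crisis state.
; A GetMissionTitle helper turns mission enums into text, naming arrest targets from a data table row.
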(event `self.ReceiveBeginPlay`
  (`parent.ReceiveBeginPlay`)
  (bind _selected (`/Game/Blueprints/Crisis/BPFL_Crisis.Bind to Crisis Selected` (delegate `On Crisis Selected`)))
  (`/Engine/EditorBlueprintResources/StandardMacros.IsValid` _selected
    (:`Is Valid`
      (`self.On Crisis Selected` _selected))))

(event `On Crisis Selected`
  (params (Comp :type "/Game/Blueprints/Crisis/BP_Crisis_Component Object Reference"))
  (if (`/Game/Blueprints/Crisis/BP_Crisis_Component.District Selected` Comp)
    (set `self.Selected Crisis Comp` Comp)))

(event `self.ReceiveTick`
  (params (DeltaSeconds :type "Float (single-precision)"))
  (bind _selected_crisis_comp (`self.Selected Crisis Comp`)
    (:`then`
      (if (>= (`/Game/Blueprints/Crisis/BP_Crisis_Component.Selected Mission` _selected_crisis_comp) 0)
        (`self.Set Title` (`|FormatText` "{NextMission}:  \n{District} - {Mission}" "NextMission" (`/Game/Blueprints/Crisis/BP_Crisis_Component.District Name` _selected_crisis_comp) (select `bool` (`|EnumEquality` (`/Game/Blueprints/Crisis/BP_Crisis_Component.Crisis State` _selected_crisis_comp) "NewEnumerator2") :`false` (`/Game/Blueprints/Crisis/BP_Crisis_Component.Get Mission Title` _selected_crisis_comp) :`true` "Objective_ArrestChieftain")))))
    (:`else`)))

(fn `Get Mission Title`
  (params (Mission :type "/Game/_Guards/UserInterface/WorldMap/E_MissionType Enum" :default "NewEnumerator0") (Arrest :type "DataTableRowHandle Structure"))
  (returns (ReturnValue :type Text))
  (bind (_datatable _rowname) (break `DataTableRowHandle` (`local.Arrest`)))
  (if (`|EnumEquality` Mission "NewEnumerator11")
    (`/Engine/EditorBlueprintResources/StandardMacros.IsValid` _datatable
      (:`Is Valid`
        (bind _returnvalue (`|GetDataTableRow` _datatable _rowname)
          (:`then`
            (return (`|FormatText` "{title} {name}s" "Arrest" (`.Name_2_14D6D417421621A9614AEFA16F089CCD` (break `/Game/Blueprints/Core/PolygonAI/Config/F_Character_Setup` _returnvalue)))))
          (:`RowNotFound`
            _)))
      (:`Is Not Valid`
        _))
    (return (`KismetTextLibrary.Conv_StringToText` (`|GetEnumeratorNameAsString` (`local.Mission`))))
    (else
      (return (`KismetTextLibrary.Conv_StringToText` (`|GetEnumeratorNameAsString` (`local.Mission`)))))))

(fn `UserConstructionScript`
  (`parent.UserConstructionScript`))