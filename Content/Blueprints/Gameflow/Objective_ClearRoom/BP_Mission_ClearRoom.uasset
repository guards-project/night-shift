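; Mission objective that completes when enough targets in a room are killed, arrested or fractured.
; After a short server-side delay, it binds to preset targets and non-hostage, non-ignored actors of target classes inside its box, plus matching gameplay marker spawns.
; Removing a target advances the count toward a total optionally capped by MaxTargets.
; Target damage or removal triggers late-start handling, so engaging targets can start the mission.
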(event `self.ReceiveBeginPlay`
  ;[1 1 1] Track ClearRoom Targets
  (`parent.ReceiveBeginPlay`)
  (`/Engine/EditorBlueprintResources/ActorMacros.Switch Has Authority`
    (:`Authority`
      (`KismetSystemLibrary.Delay` 0.2)
      (`self.Track Targets`) ; Tracking on begin play allows bindings to start the mission later if not already started
      (`self.Track Late Spawners`))))

(event `On Actor Fractured`
  (params (Actor :type "/Game/Blueprints/Fracture/FractureCore/BP_FractureActor Object Reference"))
  ;[1 1 1] Target Tracking and Late Start Mission based on any events
  (`self.Remove Target` Actor))

(event `On Enemy Died`
  (params (Character :type "/Game/Blueprints/Core/BP_Character_Template Object Reference"))
  ;[1 1 1] Target Tracking and Late Start Mission based on any events
  (`self.Remove Target` Character))

(event `On Target Damaged`
  (params (DamagedActor :type "Actor Object Reference") (Damage :type "Float (single-precision)") (DamageType :type "DamageType Object Reference") (InstigatedBy :type "Controller Object Reference") (DamageCauser :type "Actor Object Reference"))
  ;[1 1 1] Target Tracking and Late Start Mission based on any events
  (`self.Handle Late Start Mission`))

(event `BP_Mission_ClearRoom_Arrested`
  (params (Character :type "/Game/Blueprints/Core/BP_Character_Template Object Reference") (Arrested :type Boolean))
  ;[1 1 1] Target Tracking and Late Start Mission based on any events
  (if Arrested
    (`self.Remove Target` Character)))

(fn `Add Target`
  (params (`New Target` :type "Actor Object Reference (by ref)") (`Force Bind` :type Boolean))
  (bind _new_target (`local.New Target`))
  (bind _returnvalue (`KismetArrayLibrary.Array_AddUnique` (`self.Targets`) `New Target`))
  (if (or (>= _returnvalue 0) `Force Bind`)
    (`self.Targets Updated` self)
    (`|ExecutionSequence`
      (:`then_0`
        (add `self.OnTakeAnyDamage` _new_target (`|CreateDelegate` :!event `On Target Damaged`))
        (add `self.OnDestroyed` _new_target (`|CreateDelegate` :!event `Remove Target`))
        (`|ExecutionSequence`
          (:`then_0`
            (bind _asbp_character_template (cast `/Game/Blueprints/Core/BP_Character_Template` (`local.New Target`)))
            (add `/Game/Blueprints/Core/BP_Character_Template.OnDied` _asbp_character_template (`|CreateDelegate` :!event `On Enemy Died`)))
          (:`then_1`
            (bind _asbp_fracture_actor (cast `/Game/Blueprints/Fracture/FractureCore/BP_FractureActor` (`local.New Target`)))
            (add `/Game/Blueprints/Fracture/FractureCore/BP_FractureActor.Fractured` _asbp_fracture_actor (`|CreateDelegate` :!event `On Actor Fractured`)))
          (:`then_2`
            (bind _asbp_polygon_ai (cast `/Game/Blueprints/Core/PolygonAI/BP_Polygon_AI` (`local.New Target`)))
            (add `/Game/Blueprints/Core/PolygonAI/BP_Polygon_AI.On Arrested Updated` _asbp_polygon_ai (`|CreateDelegate` :!event `BP_Mission_ClearRoom_Arrested`)))))
      (:`then_1`
        (return)))))

(fn `Bind to Gameplay Markers`
  (params (`Gameplay Markers` :type "Array of /Game/Blueprints/Level/Gameplay/BP_GameplayMarker Object Reference"))
  (for _array_element `Gameplay Markers`
    (add `/Game/Blueprints/Level/Gameplay/BP_GameplayMarker.Actor Spawned` _array_element (`|CreateDelegate` :!event `On Tracked Gameplay Marker Spawned Actor`))))

(fn `Check Win`
  (returns (`Is Win` :type Boolean))
  (if (`|EnumEquality` (`self.Get Mission State`) "NewEnumerator3")
    (return (>= (`self.Current Count`) (`self.Target Count`)))
    (else
      (return false))))

(fn `On Marker Spawned Actor`
  (params (Invoker :type "/Game/Blueprints/Level/Gameplay/BP_GameplayMarker Object Reference") (`Spawned Actor` :type "Actor Object Reference"))
  (`self.Add Target` `Spawned Actor`))

(fn `On Tracked Gameplay Marker Spawned Actor`
  (params (Invoker :type "/Game/Blueprints/Level/Gameplay/BP_GameplayMarker Object Reference") (`Spawned Actor` :type "Actor Object Reference"))
  (`self.Add Target` `Spawned Actor`)
  (`self.Update Target Count`))

(fn `Remove Target`
  (params (Actor :type "Actor Object Reference"))
  (bind _returnvalue (`KismetArrayLibrary.Array_RemoveItem` (`self.Targets`) Actor))
  (if _returnvalue
    (set `self.Current Count` (+ (`self.Current Count`) 1))
    (`self.Handle Late Start Mission`)
    (bind _is_win (`self.Check Win`))
    (if _is_win
      (`self.Complete Mission` "NewEnumerator1"))))

(fn `Track Late Spawners`
  (bind _outactors (`GameplayStatics.GetAllActorsOfClass` "/Game/Blueprints/Level/Gameplay/BP_GameplayMarker.BP_GameplayMarker_C"))
  (for _array_element _outactors
    (for _array_element_2 (`self.Target Class`)
      (if (`KismetArrayLibrary.Array_Contains` (`/Game/Blueprints/Level/Gameplay/BP_GameplayMarker.Actor` _array_element) _array_element_2)
        (add `/Game/Blueprints/Level/Gameplay/BP_GameplayMarker.Actor Spawned` _array_element (`|CreateDelegate` :!event `On Marker Spawned Actor`))
        (break)))))

(fn `Track Targets`
  (bind _box (`self.Box`))
  (for _array_element (`self.Targets`)
    (`self.Add Target` _array_element true))
  (for _array_element_2 (`self.Target Class`)
    (bind _outactors (`GameplayStatics.GetAllActorsOfClass` _array_element_2))
    (for _array_element_3 _outactors
      (if (not (`KismetArrayLibrary.Array_Contains` (`self.Ignore`) _array_element_3))
        (if (!= (`GameplayStatics.GetObjectClass` _array_element_3) "/Game/Blueprints/Core/PolygonAI/BP_Polygon_AI_Hostage.BP_Polygon_AI_Hostage_C")
          (if (`KismetMathLibrary.IsPointInBoxWithTransform` (`self.K2_GetActorLocation` _array_element_3) (`SceneComponent.K2_GetComponentToWorld` _box) (`BoxComponent.BoxExtent` _box))
            (`self.Add Target` _array_element_3))))))
  (`self.Update Target Count`))

(fn `Update Target Count`
  (bind _max_targets (`self.Max Targets`))
  (bind _returnvalue (`KismetArrayLibrary.Array_Length` (`self.Targets`)))
  (set `self.Target Count` (`KismetMathLibrary.Min` (`KismetMathLibrary.SelectInt` _max_targets _returnvalue (> _max_targets 0)) _returnvalue)))

(fn `UserConstructionScript`
  (`parent.UserConstructionScript`))