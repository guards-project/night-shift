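; Room mission for the Guards mode that can end the level on a win or loss.
; On the server, a player entering its box or an overlapping door fracturing starts the countdown if the mission is unstarted.
; A result either ends the round through the game state, passing a living player's transform as context, or shows mission-complete UI.
; Level-ending wins require no active registered missions; level-ending missions skip destruction for the AAR.
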(event `self.ReceiveBeginPlay`
  ;[1 1 1] Init mission, listen to doors being kicked, players all being dead, and gather overlapping targets taking damage/dying/fracturing to start the mission if it isn't already started
  (`parent.ReceiveBeginPlay`)
  (`/Engine/EditorBlueprintResources/ActorMacros.Switch Has Authority`
    (:`Authority`
      (`KismetSystemLibrary.Delay` 0.2) ; This delay allows other actors to init\nso that box.overlappingactors works
      (`self.Track Overlapping Doors`))))

(event `self.On Mission State Changed`
  (params (`Mission State` :type "/Game/Primer/Primer_MissionHierarchy/E_MissionState Enum" :default "NewEnumerator6"))
  ;[1 1 1] On Client state changed
  (`parent.On Mission State Changed` `Mission State`)
  (switch `/Game/Primer/Primer_MissionHierarchy/E_MissionState` `Mission State`
    (:`NewEnumerator1`
      _)
    (:`NewEnumerator2`
      _))
  (`/Engine/EditorBlueprintResources/StandardMacros.DoOnce` false
    (:`Completed`
      (if (`self.Is End of Level`)
        (`/Engine/EditorBlueprintResources/ActorMacros.Switch Has Authority`
          (:`Authority`
            (`self.Set Win Context`)
            (bind _asbp_game_state_guards (cast `/Game/Blueprints/Core/BP_GameState_Guards` (`GameplayStatics.GetGameState`)))
            (`/Game/Blueprints/Core/BP_GameState_Guards.MC End Round` _asbp_game_state_guards (`|EnumEquality` (`self.Get Mission State`) "NewEnumerator1") (`self.Context`) (`self.Duration Expired`))))
        (else
          (bind _returnvalue (`|CreateWidget` (`self.Mission Complete UI`) null self))
          (`UserWidget.AddToViewport` _returnvalue 0))))))

(event `self.Box.OnComponentBeginOverlap`
  (params (OverlappedComponent :type "PrimitiveComponent Object Reference") (OtherActor :type "Actor Object Reference") (OtherComp :type "PrimitiveComponent Object Reference") (OtherBodyIndex :type Integer) (bFromSweep :type Boolean) (SweepResult :type "HitResult Structure (by ref)"))
  ;[1 1 1] Player Overlap - Start mission if it isn't already
  (cast `/Game/Blueprints/Core/BP_Character_Template_Player` OtherActor)
  (`/Engine/EditorBlueprintResources/StandardMacros.DoOnce` false
    (:`Completed`
      (`|ExecutionSequence`
        (:`then_1`
          (`self.Handle Late Start Mission`))))))

(event `On Door Fractured`
  (params (Actor :type "/Game/Blueprints/Fracture/FractureCore/BP_FractureActor Object Reference"))
  ;[1 1 1] Start the mission if a door in the area exploded!
  (`self.Handle Late Start Mission`))

(event `self.Post Complete Destroy`
  ;[1 1 1] Stop destroy if its the last mission so the AAR can read it
  (if (not (`self.Is End of Level`))
    (`parent.Post Complete Destroy`)))

(event `self.Duration Complete`
  ;[1 1 1] Setup timeout context camera
  (`self.Set Timeout Context`)
  (set `self.Duration Expired` true)
  (`parent.Duration Complete`))

(fn `Get All Rooms Complete`
  (returns (`All Rooms Complete` :type Boolean))
  (for _array_element (`/Game/Primer/Primer_MissionHierarchy/BP_MissionRegistry_Component.Registered Missions` (`self.Mission Registry`))
    (if (`|EnumEquality` (`self.Get Mission State` _array_element) "NewEnumerator3")
      (return false)))
  (return true))

(fn `Get Living Player Location`
  (returns (ReturnValue :type "Transform Structure (by ref)"))
  (for _array_element (`GameStateBase.PlayerArray` (`GameplayStatics.GetGameState`))
    (bind _returnvalue (`PlayerState.GetPawn` _array_element))
    (`/Engine/EditorBlueprintResources/StandardMacros.IsValid` _returnvalue
      (:`Is Valid`
        (bind _dead (message `/Game/Blueprints/Core/BPI_Character.Is Dead` _returnvalue))
        (bind _ko (message `/Game/Blueprints/Core/BPI_Character.Is KO` _returnvalue))
        (if (not (or _ko _dead))
          (return (`self.GetTransform` _returnvalue))))))
  (return))

(fn `Handle Late Start Mission`
  (`/Engine/EditorBlueprintResources/ActorMacros.Switch Has Authority`
    (:`Authority`
      (if (`|EnumEquality` (`self.Get Mission State`) "NewEnumerator6")
        (`self.Start Countdown`)))))

(fn `Is End of Level`
  (returns (ReturnValue :type Boolean))
  (return (or (and (`self.Win Ends Level`) (`self.Get All Rooms Complete`) (`|EnumEquality` (`self.Get Mission State`) "NewEnumerator1")) (and (`self.Loss Ends Level`) (`|EnumEquality` (`self.Get Mission State`) "NewEnumerator2")))))

(fn `Set Timeout Context`
  (bind _returnvalue (`self.Get Living Player Location`))
  (set `self.Context` _returnvalue)
  (return))

(fn `Set Win Context`
  (if (`|EnumInequality` (`self.Get Mission State`) "NewEnumerator2")
    (bind _returnvalue (`self.Get Living Player Location`))
    (set `self.Context` _returnvalue)
    (return)))

(fn `Track Overlapping Doors`
  (for _array_element (`PrimitiveComponent.GetOverlappingActors` (`self.Box`) "/Game/Blueprints/Fracture/Doors/BP_Fracture_Door_01.BP_Fracture_Door_01_C")
    (bind _asbp_fracture_actor (cast `/Game/Blueprints/Fracture/FractureCore/BP_FractureActor` _array_element))
    (add `/Game/Blueprints/Fracture/FractureCore/BP_FractureActor.Fractured` _asbp_fracture_actor (`|CreateDelegate` :!event `On Door Fractured`))))

(fn `UserConstructionScript`
  (`parent.UserConstructionScript`))