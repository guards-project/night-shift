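; Escort mission objective that tracks targets until enough of them overlap the BP_EscortGoal, whose marker it registers.
; The authority gathers targets from a preset list, class searches within its box and gameplay marker spawns, then binds their damage, death and fracture events.
; Arrivals raise the count toward a win, while losses can end the mission through CanContinueEscort.
; These events can also late-start the mission, and OnRep_Targets applies custom-depth highlighting to fracture actors.
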(event `Goal Overlapped`
  (params (Goal :type "/Game/Blueprints/Gameflow/Objective_Escort/BP_EscortGoal Object Reference") (Actor :type "Actor Object Reference"))
  (`self.Remove Target` Actor))

(event `Init Escort Goal`
  (bind _returnvalue (`GameplayStatics.GetActorOfClass` "/Game/Blueprints/Gameflow/Objective_Escort/BP_EscortGoal.BP_EscortGoal_C"))
  (`/Engine/EditorBlueprintResources/StandardMacros.IsValid` _returnvalue
    (:`Is Valid`
      (`/Game/Primer/Primer_Markers/BP_Marker.Register Marker` (`/Game/Blueprints/Gameflow/Objective_Escort/BP_EscortGoal.BP_Marker` _returnvalue))
      (`/Engine/EditorBlueprintResources/ActorMacros.Switch Has Authority`
        (:`Authority`
          (add `/Game/Blueprints/Gameflow/Objective_Escort/BP_EscortGoal.On Overlap` _returnvalue (delegate `Goal Overlapped`)))))
    (:`Is Not Valid`
      (`KismetSystemLibrary.K2_SetTimerDelegate` (delegate `Init Escort Goal`) 0.2))))

(event `self.ReceiveBeginPlay`
  ;[1 1 1] Track escort targets
  (`parent.ReceiveBeginPlay`)
  (`self.Init Escort Goal`)
  (`/Engine/EditorBlueprintResources/ActorMacros.Switch Has Authority`
    (:`Authority`
      (`KismetSystemLibrary.Delay` 0.2)
      (`self.Track Targets`) ; Tracking on begin play allows bindings to start the mission later if not already started
      (`self.Track Late Spawns`))))

(event `On Actor Fractured`
  (params (Actor :type "/Game/Blueprints/Fracture/FractureCore/BP_FractureActor Object Reference"))
  ;[1 1 1] Target Tracking and Late Start Mission based on any events
  (`self.Handle Late Start Mission`)
  (bind _returnvalue (`self.Stop Tracking Target` Actor))
  (if _returnvalue
    (bind _continue (`self.Can Continue Escort`))
    (if (not _continue)
      (set `self.Context` (`self.GetTransform` Actor))
      (`self.Complete Mission` "NewEnumerator2"))))

(event `On AI Died`
  (params (Character :type "/Game/Blueprints/Core/BP_Character_Template Object Reference"))
  ;[1 1 1] Target Tracking and Late Start Mission based on any events
  (`self.Handle Late Start Mission`)
  (bind _returnvalue (`self.Stop Tracking Target` Character))
  (if _returnvalue
    (bind _continue (`self.Can Continue Escort`))
    (if (not _continue)
      (set `self.Context` (`self.GetTransform` Character))
      (`self.Complete Mission` "NewEnumerator2"))))

(event `On Target Damaged`
  (params (DamagedActor :type "Actor Object Reference") (Damage :type "Float (single-precision)") (DamageType :type "DamageType Object Reference") (InstigatedBy :type "Controller Object Reference") (DamageCauser :type "Actor Object Reference"))
  ;[1 1 1] Target Tracking and Late Start Mission based on any events
  (`self.Handle Late Start Mission`))

(event `self.Complete Mission`
  (params (`Mission State` :type "/Game/Primer/Primer_MissionHierarchy/E_MissionState Enum" :default "NewEnumerator6"))
  (`parent.Complete Mission` `Mission State`)
  (bind _returnvalue (`GameplayStatics.GetActorOfClass` "/Game/Blueprints/Gameflow/Objective_Escort/BP_EscortGoal.BP_EscortGoal_C"))
  (`/Engine/EditorBlueprintResources/StandardMacros.IsValid` _returnvalue
    (:`Is Valid`
      (`/Game/Primer/Primer_Markers/BP_Marker.Unregister Marker` (`/Game/Blueprints/Gameflow/Objective_Escort/BP_EscortGoal.BP_Marker` _returnvalue)))))

(fn `Add Target`
  (params (`New Target` :type "Actor Object Reference (by ref)"))
  (bind _returnvalue (`KismetArrayLibrary.Array_AddUnique` (`self.Targets`) `New Target`))
  (if (>= _returnvalue 0)
    (`self.Bind to Target` `New Target`)))

(fn `Bind to Gameplay Markers`
  (params (`Gameplay Markers` :type "Array of /Game/Blueprints/Level/Gameplay/BP_GameplayMarker Object Reference"))
  (bind _output_get (set `self.Gameplay Markers` `Gameplay Markers`))
  (for _array_element _output_get
    (bind _last_spawned_actor (`/Game/Blueprints/Level/Gameplay/BP_GameplayMarker.Last Spawned Actor` _array_element)
      (:`then`
        (`self.On Tracked Gameplay Marker Spawned Actor` null _last_spawned_actor)
        (`KismetSystemLibrary.PrintString` (`KismetSystemLibrary.GetDisplayName` _last_spawned_actor)))
      (:`else`
        (add `/Game/Blueprints/Level/Gameplay/BP_GameplayMarker.Actor Spawned` _array_element (`|CreateDelegate` :!event `On Tracked Gameplay Marker Spawned Actor`))))))

(fn `Bind to Target`
  (params (Target :type "Actor Object Reference"))
  (bind _target (`local.Target`))
  (`self.Targets Updated` self)
  (`|ExecutionSequence`
    (:`then_0`
      (add `self.OnTakeAnyDamage` Target (`|CreateDelegate` :!event `On Target Damaged`))
      (add `self.OnDestroyed` (`|CreateDelegate` :!event `Remove Target`))
      (`|ExecutionSequence`
        (:`then_0`
          (bind _asbp_character_template (cast `/Game/Blueprints/Core/BP_Character_Template` _target))
          (add `/Game/Blueprints/Core/BP_Character_Template.OnDied` _asbp_character_template (`|CreateDelegate` :!event `On AI Died`))
          (return))
        (:`then_1`
          (bind _asbp_fracture_actor (cast `/Game/Blueprints/Fracture/FractureCore/BP_FractureActor` _target))
          (add `/Game/Blueprints/Fracture/FractureCore/BP_FractureActor.Fractured` _asbp_fracture_actor (`|CreateDelegate` :!event `On Actor Fractured`))
          (return))
        (:`then_2`
          (bind _asbp_gameplay_marker (cast `/Game/Blueprints/Level/Gameplay/BP_GameplayMarker` _target))
          (`KismetArrayLibrary.Array_RemoveItem` (`self.Targets`) (`local.Target`))
          (bind _last_spawned_actor (`/Game/Blueprints/Level/Gameplay/BP_GameplayMarker.Last Spawned Actor` _asbp_gameplay_marker)
            (:`then`
              (`self.On Tracked Gameplay Marker Spawned Actor` _asbp_gameplay_marker _last_spawned_actor))
            (:`else`
              (add `/Game/Blueprints/Level/Gameplay/BP_GameplayMarker.Actor Spawned` _asbp_gameplay_marker (`|CreateDelegate` :!event `On Tracked Gameplay Marker Spawned Actor`))))
          (return))))
    (:`then_1`
      (return))))

(fn `Can Continue Escort`
  (returns (Continue :type Boolean))
  (if (<= (`self.Max Targets`) 0)
    (return false)
    (else
      (return (>= (`KismetArrayLibrary.Array_Length` (`self.Targets`)) (- (`self.Max Targets`) (`self.Current Count`)))))))

(fn `Check Win`
  (returns (`Is Win` :type Boolean))
  (if (`|EnumEquality` (`self.Get Mission State`) "NewEnumerator3")
    (return (>= (`self.Current Count`) (`self.Target Count`)))
    (else
      (return false))))

(fn `On Tracked Gameplay Marker Spawned Actor`
  (params (Invoker :type "/Game/Blueprints/Level/Gameplay/BP_GameplayMarker Object Reference") (`Spawned Actor` :type "Actor Object Reference"))
  (`self.Add Target` `Spawned Actor`)
  (`self.Update Target Count`))

(fn `OnRep_Targets`
  (`self.Targets Updated` self)
  (for _array_element (`self.Targets`)
    (bind _asbp_fracture_actor (cast `/Game/Blueprints/Fracture/FractureCore/BP_FractureActor` _array_element))
    (bind _item_mesh (`/Game/Blueprints/Items/BP_Item.Item Mesh` _asbp_fracture_actor))
    (`PrimitiveComponent.SetRenderCustomDepth` _item_mesh true)
    (`PrimitiveComponent.SetCustomDepthStencilValue` _item_mesh 2)))

(fn `Remove Target`
  (params (Actor :type "Actor Object Reference"))
  (bind _returnvalue (`self.Stop Tracking Target` Actor))
  (if _returnvalue
    (`self.Targets Updated` self)
    (set `self.Current Count` (+ (`self.Current Count`) 1))
    (`self.Handle Late Start Mission`)
    (`|ExecutionSequence`
      (:`then_0`
        (bind _asbp_polygon_ai_chief (cast `/Game/Blueprints/Core/PolygonAI/BP_Polygon_AI_Chief` (`local.Actor`))
          (:`CastFailed`
            (bind _asai_controller_polygon (cast `/Game/Blueprints/Core/PolygonAI/Behaviour/AI_Controller_Polygon` (`AIBlueprintHelperLibrary.GetAIController` _asbp_polygon_ai_chief)))
            (`/Game/Blueprints/Core/PolygonAI/Behaviour/AI_Controller_Polygon.Set BB AI State` _asai_controller_polygon "NewEnumerator4") ; make the follow ai retreat upon reaching the goal
          )))
      (:`then_1`
        (bind _is_win (`self.Check Win`))
        (if _is_win
          (`self.Complete Mission` "NewEnumerator1"))))))

(fn `Set Timeout Context`
  (set `self.Context` (`self.GetTransform` (`KismetArrayLibrary.Array_Random` (`self.Targets`)))))

(fn `Stop Tracking Target`
  (params (Item :type "Actor Object Reference (by ref)"))
  (returns (ReturnValue :type Boolean))
  (bind _returnvalue (`KismetArrayLibrary.Array_RemoveItem` (`self.Targets`) Item))
  (if _returnvalue
    (`KismetSystemLibrary.PrintString` (`KismetSystemLibrary.GetDisplayName` Item) true true (struct :`R` 0.814847 :`G` 0.021219 :`B` 0.021219 :`A` 1.0))
    (set `self.Targets` (`self.Targets`)) ; force update
    (return true)
    (else
      (return false))))

(fn `Track Late Spawns`
  (bind _outactors (`GameplayStatics.GetAllActorsOfClass` "/Game/Blueprints/Level/Gameplay/BP_GameplayMarker.BP_GameplayMarker_C"))
  (for _array_element _outactors
    (for _array_element_2 (`self.Target Class`)
      (if (`KismetArrayLibrary.Array_Contains` (`/Game/Blueprints/Level/Gameplay/BP_GameplayMarker.Actor` _array_element) _array_element_2)
        (add `/Game/Blueprints/Level/Gameplay/BP_GameplayMarker.Actor Spawned` _array_element (`|CreateDelegate` :!event `On Tracked Gameplay Marker Spawned Actor`))
        (break)))))

(fn `Track Targets`
  (bind _box (`self.Box`))
  (for _array_element (`self.Targets`)
    (`self.Bind to Target` _array_element))
  (for _array_element_2 (`self.Target Class`)
    (bind _outactors (`GameplayStatics.GetAllActorsOfClass` _array_element_2))
    (for _array_element_3 _outactors
      (if (`KismetMathLibrary.IsPointInBoxWithTransform` (`self.K2_GetActorLocation` _array_element_3) (`SceneComponent.K2_GetComponentToWorld` _box) (`BoxComponent.BoxExtent` _box))
        (`self.Add Target` _array_element_3))))
  (`self.Update Target Count`))

(fn `Update Target Count`
  (bind _max_targets (`self.Max Targets`))
  (bind _returnvalue (`KismetArrayLibrary.Array_Length` (`self.Targets`)))
  (set `self.Target Count` (`KismetMathLibrary.Min` (`KismetMathLibrary.SelectInt` _max_targets _returnvalue (> _max_targets 0)) _returnvalue)))

(fn `UserConstructionScript`
  (`parent.UserConstructionScript`))