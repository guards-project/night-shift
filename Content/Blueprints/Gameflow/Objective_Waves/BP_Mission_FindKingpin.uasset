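; Mission objective for finding the Kingpin, completed once when a player overlaps its box.
; Before activating follow-up missions, it plays an offset level sequence with HUD, player and input disabled, while the server teleports players to random navmesh points around an arrow.
; After a delay, it triggers "Kingpin"-tagged gameplay markers and tags the spawned AI as "Boss".
; When the sequence ends, it restores the UI, repossesses the player to fix the camera, and the server destroys the actor.
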(event `self.Box.OnComponentBeginOverlap`
  (params (OverlappedComponent :type "PrimitiveComponent Object Reference") (OtherActor :type "Actor Object Reference") (OtherComp :type "PrimitiveComponent Object Reference") (OtherBodyIndex :type Integer) (bFromSweep :type Boolean) (SweepResult :type "HitResult Structure (by ref)"))
  (if (`self.ActorHasTag` OtherActor "Player")
    (`/Engine/EditorBlueprintResources/StandardMacros.DoOnce` false
      (:`Completed`
        (`self.Complete Mission` "NewEnumerator1")))))

(event `self.Activate Next Missions`
  (`self.MC_Sequence`)
  (`KismetSystemLibrary.Delay` 1.5)
  (`parent.Activate Next Missions`))

(event `MC_Sequence`
  (bind (_returnvalue_roll _returnvalue_pitch _returnvalue_yaw) (`KismetMathLibrary.BreakRotator` (`SceneComponent.K2_GetComponentRotation` (`self.Player Teleport Arrow`))))
  (bind _returnvalue (`KismetMathLibrary.MakeRotator` 0.0 0.0 _returnvalue_yaw))
  (bind _output (`/Game/_Guards/UserInterface/Menus/Stack/BPFL_CommonStack.Get Common Widget Stack`))
  (`Widget.SetVisibility` _output "Hidden")
  (bind (_outactor _returnvalue_2) (`LevelSequencePlayer.CreateLevelSequencePlayer` (`self.Level Sequence`) (make `MovieSceneSequencePlaybackSettings` false (struct) 1.0 0.0 false true true true true true)))
  (set `LevelSequenceActor.bOverrideInstanceData` true _outactor)
  (add `MovieSceneSequencePlayer.OnFinished` _returnvalue_2 (delegate `OnFinished_Event`))
  (bind _asdefault_level_sequence_instance_data (cast `DefaultLevelSequenceInstanceData` (`LevelSequenceActor.DefaultInstanceData` _outactor)))
  (set `DefaultLevelSequenceInstanceData.TransformOrigin` (`KismetMathLibrary.MakeTransform` (0.0 0.0 1500.0)) _asdefault_level_sequence_instance_data)
  (`MovieSceneSequencePlayer.Play` _returnvalue_2)
  (`|ExecutionSequence`
    (:`then_0`
      (`KismetSystemLibrary.Delay` 0.5)
      (`/Engine/EditorBlueprintResources/ActorMacros.Switch Has Authority`
        (:`Authority`
          (bind _outactors (`GameplayStatics.GetAllActorsOfClass` "/Game/Blueprints/Core/BP_Character_Template_Player.BP_Character_Template_Player_C"))
          (for _array_element _outactors
            (`Controller.SetControlRotation` (`Pawn.GetController` _array_element) _returnvalue)
            (`self.K2_TeleportTo` _array_element (`NavigationSystemV1.K2_GetRandomReachablePointInRadius` (`NavigationSystemV1.K2_ProjectPointToNavigation` (`SceneComponent.K2_GetComponentLocation` (`self.Player Teleport Arrow`)) null null (300.0 300.0 1000.0)) (`self.Player Teleport Radius`) null null) _returnvalue)))))
    (:`then_1`
      (`KismetSystemLibrary.Delay` (`self.Delay Kingpin Spawn`))
      (`self.Spawn Kingpin`))))

(event `OnFinished_Event`
  (`|ExecutionSequence`
    (:`then_0`
      (`/Engine/EditorBlueprintResources/ActorMacros.Switch Has Authority`
        (:`Authority`
          (`KismetSystemLibrary.Delay` 4.0)
          (`self.K2_DestroyActor`))))
    (:`then_1`
      ;[1 1 1] fixes camera issue
      (bind _output (`/Game/_Guards/UserInterface/Menus/Stack/BPFL_CommonStack.Get Common Widget Stack`))
      (`Widget.SetVisibility` _output "SelfHitTestInvisible")
      (bind _asbp_player_controller_template (cast `/Game/Blueprints/Core/BP_PlayerController_Template` (`GameplayStatics.GetPlayerController` 0)))
      (`/Game/Blueprints/Core/BP_PlayerController_Template.Server Repossess` _asbp_player_controller_template))))

(event `Spawn Kingpin`
  (bind _outactors (`GameplayStatics.GetAllActorsWithTag` "Kingpin"))
  (for _array_element _outactors
    (bind _asbp_gameplay_marker (cast `/Game/Blueprints/Level/Gameplay/BP_GameplayMarker` _array_element))
    (add `/Game/Blueprints/Level/Gameplay/BP_GameplayMarker.Actor Spawned` _asbp_gameplay_marker (delegate `Actor Spawned_Event`))
    (message `/Game/Primer/Primer_Shared/BPI_Activation.Trigger Activate` _array_element self)))

(event `Actor Spawned_Event`
  (params (Invoker :type "/Game/Blueprints/Level/Gameplay/BP_GameplayMarker Object Reference") (`Spawned Actor` :type "Actor Object Reference"))
  (bind _asbp_polygon_ai (cast `/Game/Blueprints/Core/PolygonAI/BP_Polygon_AI` `Spawned Actor`))
  (`KismetSystemLibrary.Delay` 0.2)
  (set `Actor.Tags` (`|MakeArray` "Boss" :!type "Name") _asbp_polygon_ai))

(fn `UserConstructionScript`
  (`parent.UserConstructionScript`))