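; Wave-survival mission objective that completes once the enemies of every wave are killed, arrested or destroyed.
; The server activates a shuffled, count-limited set of spawners found by comma-separated wave tags, falling back to "EnemySpawner".
; Spawned AI are tracked, alerted and sent along a path, with movement re-enabled on equipment changes.
; Clearing a wave starts a timer for the next, with replicated NextWaveTime driving the countdown widget.
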(event `self.Start Mission`
  ;[1 1 1] Begin
  (`parent.Start Mission`)
  (`/Engine/EditorBlueprintResources/ActorMacros.Switch Has Authority`
    (:`Authority`
      (set `self.Target Count` (`KismetArrayLibrary.Array_Length` (`self.Wave Tags`)))
      (`self.Bind to Wave Spawns`)
      (`KismetSystemLibrary.Delay` 0.3)
      (`self.Activate Next Wave`))))

(event `MC On Wave Started`
  ;[1 1 1] Begin
  (`/Engine/EditorBlueprintResources/StandardMacros.Can Execute Cosmetic Events`
    (:`True`
      (`GameplayStatics.PlaySound2D` "/Game/Blueprints/Gameflow/Objective_Waves/A_WarHorn.A_WarHorn" 1.0 1.0 0.0 null null))))

(fn `Activate Next Wave`
  (locals (`L Actors` :type "Array of Actor Object Reference"))
  (bind _l_actors (`local.L Actors`))
  (if (`KismetArrayLibrary.Array_IsEmpty` (`self.Wave Tags`))
    (bind _outactors (`GameplayStatics.GetAllActorsWithTag` "EnemySpawner")) ; Fallback
    (`KismetArrayLibrary.Array_Append` (`local.L Actors`) _outactors)
    (else
      (for _array_element (`self.Comma Seperate Wave Tags` (`|GetArrayItem` (`self.Wave Tags`)))
        (bind _outactors_2 (`GameplayStatics.GetAllActorsWithTag` _array_element))
        (`KismetArrayLibrary.Array_Append` (`local.L Actors`) _outactors_2))))
  (`KismetArrayLibrary.Array_Shuffle` _l_actors)
  (`KismetArrayLibrary.Array_Resize` _l_actors (`KismetMathLibrary.Min` (`|GetArrayItem` (`self.Enemy Counts`)) (`KismetArrayLibrary.Array_Length` (`local.L Actors`))))
  (message `/Game/Primer/Primer_Shared/BPI_Activation.Trigger Activate` (`local.L Actors`) self)
  (`self.MC On Wave Started`)
  (set `self.Enemy Count` (`KismetArrayLibrary.Array_Length` (`local.L Actors`)))
  (set `self.Enemies Subdued` 0)
  (set `self.Wave Targets` (`local.L Actors`)))

(fn `Bind to Wave Spawns`
  (if (`KismetArrayLibrary.Array_IsEmpty` (`self.Wave Tags`))
    (bind _outactors (`GameplayStatics.GetAllActorsWithTag` "EnemySpawner")) ; Fallback
    (for _array_element _outactors
      (bind _asbp_gameplay_marker (cast `/Game/Blueprints/Level/Gameplay/BP_GameplayMarker` _array_element))
      (add `/Game/Blueprints/Level/Gameplay/BP_GameplayMarker.Actor Spawned` _asbp_gameplay_marker (`|CreateDelegate` :!event `On Wave Actor Spawned`)))
    (else
      (for _array_element_2 (`self.Wave Tags`)
        (for _array_element_3 (`self.Comma Seperate Wave Tags` _array_element_2)
          (bind _outactors_2 (`GameplayStatics.GetAllActorsWithTag` _array_element_3))
          (for _array_element_4 _outactors_2
            (bind _asbp_gameplay_marker_2 (cast `/Game/Blueprints/Level/Gameplay/BP_GameplayMarker` _array_element_4))
            (add `/Game/Blueprints/Level/Gameplay/BP_GameplayMarker.Actor Spawned` _asbp_gameplay_marker_2 (`|CreateDelegate` :!event `On Wave Actor Spawned`))))))))

(fn `Check Win`
  (returns (`Is Win` :type Boolean))
  (if (`|EnumEquality` (`self.Get Mission State`) "NewEnumerator3")
    (return (`KismetArrayLibrary.Array_IsEmpty` (`self.Wave Tags`)))
    (else
      (return false))))

(fn `Comma Seperate Wave Tags`
  (params (`In Tags` :type Name))
  (returns (`Out Tags` :type "Array of Name"))
  (locals (`L Out Tags` :type "Array of Name"))
  (for _array_element (`KismetStringLibrary.ParseIntoArray` (`KismetStringLibrary.Conv_NameToString` `In Tags`) ",")
    (`KismetArrayLibrary.Array_Add` (`local.L Out Tags`) (`KismetStringLibrary.Conv_StringToName` _array_element)))
  (return (`local.L Out Tags`)))

(fn `On AI Arrested Changed`
  (params (Character :type "/Game/Blueprints/Core/BP_Character_Template Object Reference") (Arrested :type Boolean))
  (if Arrested
    (`self.Remove Active Enemy` Character)))

(fn `On AI Changed Equipment`
  (params (Mainhand :type "/Game/Blueprints/Items/BP_Item Object Reference") (Offhand :type "/Game/Blueprints/Items/BP_Item Object Reference"))
  (bind _returnvalue (`self.GetOwner` Mainhand))
  ;[1 1 1] Override the Thrower / Ranged ai behaviour to stand still
  (`/Engine/EditorBlueprintResources/StandardMacros.IsValid` Mainhand
    (:`Is Valid`
      (`/Engine/EditorBlueprintResources/StandardMacros.IsValid` _returnvalue
        (:`Is Valid`
          (bind _asbp_polygon_ai (cast `/Game/Blueprints/Core/PolygonAI/BP_Polygon_AI` _returnvalue))
          (`/Game/Blueprints/Core/BP_Character_Template.Auth Set Can Move` _asbp_polygon_ai true))))))

(fn `On Enemy Destroyed`
  (params (DestroyedActor :type "Actor Object Reference"))
  (bind _asbp_character_template (cast `/Game/Blueprints/Core/BP_Character_Template` DestroyedActor))
  (`self.Remove Active Enemy` _asbp_character_template))

(fn `On Enemy Reached Path Node`
  (params (`AI Character` :type "/Game/Blueprints/Core/PolygonAI/BP_Polygon_AI Object Reference"))
  (`/Game/Blueprints/Core/BP_Character_Template.Auth Set Move State` (`local.AI Character`) (`BlueprintMapLibrary.Map_Find` (`.MoveSetup_43_970037874107B618C5D7A7B3D444E862` (break `/Game/Blueprints/Core/PolygonAI/Config/F_Character_Setup` (`/Game/Blueprints/Core/BP_Character_Template.Config Data` `AI Character`))) "NewEnumerator2")))

(fn `On Enemy Subdued`
  (params (Character :type "/Game/Blueprints/Core/BP_Character_Template Object Reference"))
  (`self.Remove Active Enemy` Character))

(fn `On Wave Actor Spawned`
  (params (Invoker :type "/Game/Blueprints/Level/Gameplay/BP_GameplayMarker Object Reference") (`Spawned Actor` :type "Actor Object Reference"))
  (locals (`L AI Pawn` :type "/Game/Blueprints/Core/PolygonAI/BP_Polygon_AI Object Reference"))
  (bind _l_ai_pawn (`local.L AI Pawn`))
  (bind _wave_targets (`self.Wave Targets`))
  (bind _l_ai_pawn_2 (`local.L AI Pawn`))
  (bind _l_ai_pawn_3 (`local.L AI Pawn`))
  (bind _asbp_polygon_ai (cast `/Game/Blueprints/Core/PolygonAI/BP_Polygon_AI` `Spawned Actor`))
  (set `local.L AI Pawn` _asbp_polygon_ai)
  (`KismetArrayLibrary.Array_AddUnique` (`self.Active Enemies`) (`local.L AI Pawn`))
  (add `/Game/Blueprints/Core/BP_Character_Template.OnDied` _l_ai_pawn (`|CreateDelegate` :!event `On Enemy Subdued`))
  (add `/Game/Blueprints/Core/PolygonAI/BP_Polygon_AI.On Arrested Updated` _l_ai_pawn (`|CreateDelegate` :!event `On AI Arrested Changed`))
  (add `self.OnDestroyed` _l_ai_pawn (`|CreateDelegate` :!event `On Enemy Destroyed`))
  (add `/Game/Blueprints/Items/BP_Inventory_Component.OnEquippedItemChanged` (`/Game/Blueprints/Core/BP_Character_Template.BP_Inventory_Component` _l_ai_pawn_2) (`|CreateDelegate` :!event `On AI Changed Equipment`))
  (add `/Game/Blueprints/Core/PolygonAI/BP_Polygon_AI.Path Complete` _l_ai_pawn_2 (`|CreateDelegate` :!event `On Enemy Reached Path Node`))
  (set `/Game/Blueprints/Core/PolygonAI/BP_Polygon_AI.Path Node` (`self.Path Node`) _l_ai_pawn_3)
  (bind _asai_controller_polygon (cast `/Game/Blueprints/Core/PolygonAI/Behaviour/AI_Controller_Polygon` (`AIBlueprintHelperLibrary.GetAIController` _l_ai_pawn_3)))
  (set `/Game/Blueprints/Core/PolygonAI/Behaviour/AI_Controller_Polygon.Is Alert` true _asai_controller_polygon)
  (`/Game/Blueprints/Core/BP_Character_Template.Auth Set Can Move` (`local.L AI Pawn`) true)
  (`/Game/Blueprints/Core/PolygonAI/Behaviour/AI_Controller_Polygon.Init Path` _asai_controller_polygon)
  (`/Game/Blueprints/Core/BP_Character_Template.Auth Set Move State` (`local.L AI Pawn`) (select `bool` (`|EnumEquality` (`BlueprintMapLibrary.Map_Find` (`.MoveSetup_43_970037874107B618C5D7A7B3D444E862` (break `/Game/Blueprints/Core/PolygonAI/Config/F_Character_Setup` (`/Game/Blueprints/Core/BP_Character_Template.Config Data` _l_ai_pawn))) "NewEnumerator3") "NewEnumerator2") :`false` "NewEnumerator1" :`true` "NewEnumerator2" :!type "/Game/Blueprints/Core/E_MoveState Enum"))
  (`KismetArrayLibrary.Array_AddUnique` _wave_targets (`local.L AI Pawn`))
  (set `self.Enemy Count` (`KismetArrayLibrary.Array_Length` _wave_targets)))

(fn `On Wave Complete`
  (`KismetArrayLibrary.Array_Remove` (`self.Wave Tags`))
  (`KismetArrayLibrary.Array_Remove` (`self.Enemy Counts`))
  (set `self.Current Count` (- (`self.Target Count`) (`KismetArrayLibrary.Array_Length` (`self.Wave Tags`))))
  (if (`KismetArrayLibrary.Array_IsEmpty` (`self.Wave Tags`))
    (`self.Complete Mission` "NewEnumerator1")
    (else
      (`KismetSystemLibrary.K2_SetTimerDelegate` (`|CreateDelegate` :!event `Activate Next Wave`) (`self.Delay Between Waves`))
      (set `self.NextWaveTime` (+ (`GameStateBase.GetServerWorldTimeSeconds` (`GameplayStatics.GetGameState`)) (`self.Delay Between Waves`))))))

(fn `OnRep_NextWaveTime`
  (`self.CountdownStarted`)
  (`/Engine/EditorBlueprintResources/StandardMacros.Can Execute Cosmetic Events`
    (:`True`
      (bind _returnvalue (`|CreateWidget` "/Game/_Guards/UserInterface/Missions/W_WaveComplete.W_WaveComplete_C" null self))
      (`UserWidget.AddToViewport` _returnvalue 0))))

(fn `Remove Active Enemy`
  (params (Item :type "/Game/Blueprints/Core/BP_Character_Template Object Reference (by ref)"))
  (bind _returnvalue (`KismetArrayLibrary.Array_RemoveItem` (`self.Active Enemies`) Item))
  (if _returnvalue
    (set `self.Enemies Subdued` (+ (`self.Enemies Subdued`) 1))
    (if (`KismetArrayLibrary.Array_IsEmpty` (`self.Active Enemies`))
      (`self.On Wave Complete`))))

(fn `Set Timeout Context`
  (set `self.Context` (`self.GetTransform` (`KismetArrayLibrary.Array_Random` (`self.Active Enemies`)))))

(fn `UserConstructionScript`
  (`parent.UserConstructionScript`))