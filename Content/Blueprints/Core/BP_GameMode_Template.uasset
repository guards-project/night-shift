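; Template game mode that relays player join and leave events and holds back pawn spawning while a dungeon loads.
; Login and logout fire a callback on the mode and multicast-style calls on the GameState's BP_PlayerJoinLeaveCallback component.
; When a BP_Dungeon_Manager exists, the default pawn class requires it to be loaded and spawning requires the player controller's DungeonReady flag.
; A failed spawn retries at a random PlayerStart.
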(event EventPostLogin
  (params (NewPlayer :type Player%20Controller%20Object%20Reference))
  (bind _playerstate (Variables|/Script/Engine.Controller|GetPlayerState NewPlayer))
  (Default|CallPlayerJoined (Variables|Default|GetBP_PlayerJoinLeaveCallback) NewPlayer _playerstate)
  (Default|MCJoined (Actor|GetComponentbyClass (Game|GetGameState) "/Game/Blueprints/Core/Components/BP_PlayerJoinLeaveCallback.BP_PlayerJoinLeaveCallback_C") NewPlayer _playerstate))

(event EventOnLogout
  (params (ExitingController :type Controller%20Object%20Reference))
  (bind _playerstate (Variables|/Script/Engine.Controller|GetPlayerState ExitingController))
  (Default|CallPlayerLeft (Variables|Default|GetBP_PlayerJoinLeaveCallback) ExitingController _playerstate)
  (Default|MCLeft (Actor|GetComponentbyClass (Game|GetGameState) "/Game/Blueprints/Core/Components/BP_PlayerJoinLeaveCallback.BP_PlayerJoinLeaveCallback_C") ExitingController _playerstate))

(fn ConstructionScript)

(fn GetDefaultPawnClassforController
  (params (InController :type Controller%20Object%20Reference))
  (bind _returnvalue (|CallParentFunction InController))
  (bind _returnvalue_2 (Actor|GetActorOfClass "/Game/PCG/DungeonArchitect/BP_Dungeon_Manager.BP_Dungeon_Manager_C"))
  (Utilities|IsValid _returnvalue_2
    (:Is%20Valid
      (if (Variables|/Game/PCG/DungeonArchitect/BP_Dungeon_Manager.BP_Dungeon_Manager_C|GetIs%20Loaded _returnvalue_2)
        _
        (else
          (return 0))))
    (:Is%20Not%20Valid
      _))
  (return _returnvalue))

(fn SpawnDefaultPawnatTransform
  (params (NewPlayer :type Controller%20Object%20Reference) (SpawnTransform :type Transform%20%28by%20ref%29))
  (bind _returnvalue (Actor|GetActorOfClass "/Game/PCG/DungeonArchitect/BP_Dungeon_Manager.BP_Dungeon_Manager_C"))
  (Utilities|IsValid _returnvalue
    (:Is%20Valid
      (bind _asbp_player_controller_template (Utilities|Casting|CastToBP_PlayerController_Template NewPlayer))
      (if (Variables|/Game/Blueprints/Core/BP_PlayerController_Template.BP_PlayerController_Template_C|GetDungeon%20Ready _asbp_player_controller_template)
        _
        (else
          (return 0))))
    (:Is%20Not%20Valid
      _))
  (bind _returnvalue_2 (|CallParentFunction NewPlayer SpawnTransform))
  (Utilities|IsValid _returnvalue_2
    (:Is%20Valid
      (return _returnvalue_2))
    (:Is%20Not%20Valid
      (bind _outactors (Actor|GetAllActorsOfClass "/Script/Engine.PlayerStart"))
      (bind _returnvalue_3 (|CallParentFunction NewPlayer (Transformation|GetActorTransform (.OutItem (Utilities|Array|Random _outactors)))))
      (return _returnvalue_3))))