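; Template player controller handling respawning, player actions and debug controls.
; An authority-side timer restarts the player until a pawn exists, and pawn destruction or dungeon-ready changes trigger restarts.
; Input drives voice chat, an admin photo-mode camera and debug lighting, time and weather switches; server events fund districts, apply crisis abilities and move pawns.
; Position reset samples expanding navmesh radii, accepting points with full paths to random PlayerStarts to avoid out-of-bounds teleports.
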(event Custom|Client%20Kicked
  (params (Title :type Text) (Reason :type Text))
  (bind _asbp_game_instance_template (Utilities|Casting|CastToBP_GameInstance_Template (Game|GetGameInstance)))
  (Default|SetKickReason _asbp_game_instance_template Title Reason)
  (Game|OpenLevel(byName) "EntryMap"))

(event Custom|OnDestroyed_Event
  (params (DestroyedActor :type Actor%20Object%20Reference))
  (Utilities|FlowControl|Delay 0.2)
  (Class|GameModeBase|RestartPlayer (Game|GetGameMode) self))

(event Custom|Toggle%20Admin%20Camera
  (params (Enter :type Boolean))
  ;[1 1 1] Enter/Exit
  (if Enter
    (Variables|/Script/Engine.Actor|SetbCanBeDamaged (Pawn|GetControlledPawn) false) ; guard
    (Default|EnterPhotoMode (Variables|Default|GetBP_PhotoModeComponent))
    (else
      (Default|ExitPhotoMode (Variables|Default|GetBP_PhotoModeComponent))
      (Utilities|FlowControl|Delay 0.2)
      (Variables|/Script/Engine.Actor|SetbCanBeDamaged (Pawn|GetControlledPawn) true) ; guard
    )))

(event Custom|Set%20Chatting
  (params (Chat :type Boolean))
  (bind _playerstate (Variables|GetPlayerState)
    (:then
      (Default|SetChatting (Actor|GetComponentbyClass _playerstate "/Game/Blueprints/Core/Components/Voice/BP_Voip_Component.BP_Voip_Component_C") Chat))
    (:else)))

(event Custom|Server%20Set%20Location
  (params (NewLocation :type Vector))
  (Transformation|SetActorLocation (Pawn|GetControlledPawn) NewLocation false false))

(event Custom|Flip%20Admin%20Cam
  ;[1 1 1] Enter/Exit
  (bind _foundwidgets (Widget|GetAllWidgetsOfClass "/Game/PCG/DungeonArchitect/W_LoadingDungeon.W_LoadingDungeon_C" true))
  (if (Utilities|Array|IsEmpty _foundwidgets)
    (bind _isa (Utilities|FlowControl|FlipFlop)
      (:A
        _)
      (:B
        _))
    (CallFunction|ToggleAdminCamera _isa)))

(event Custom|Check%20for%20Pawn
  (Utilities|IsValid (Pawn|GetControlledPawn)
    (:Is%20Valid
      (Utilities|Time|ClearandInvalidateTimerbyHandle (Variables|Default|GetPawn%20Check)))
    (:Is%20Not%20Valid
      (Class|GameModeBase|RestartPlayer (Game|GetGameMode) self))))

(event Custom|Server%20Change%20Weather
  (bind _returnvalue (Actor|GetActorOfClass "/Game/UltraDynamicSky/Blueprints/Ultra_Dynamic_Weather.Ultra_Dynamic_Weather_C"))
  (Utilities|IsValid _returnvalue
    (:Is%20Valid
      (Default|RandomizeWeather (Variables|/Game/UltraDynamicSky/Blueprints/Ultra_Dynamic_Weather.Ultra_Dynamic_Weather_C|GetRandom_Weather_Variation _returnvalue)))))

(event Custom|Server%20Change%20Time
  (bind _returnvalue (Actor|GetActorOfClass "/Game/UltraDynamicSky/Blueprints/Ultra_Dynamic_Sky.Ultra_Dynamic_Sky_C"))
  (Utilities|IsValid _returnvalue
    (:Is%20Valid
      (Variables|/Game/UltraDynamicSky/Blueprints/Ultra_Dynamic_Sky.Ultra_Dynamic_Sky_C|SetTime%20of%20Day _returnvalue (select (> (+ (Variables|/Game/UltraDynamicSky/Blueprints/Ultra_Dynamic_Sky.Ultra_Dynamic_Sky_C|GetTime%20of%20Day _returnvalue) 5e+01) 2.4e+03) 0.0 (+ (Variables|/Game/UltraDynamicSky/Blueprints/Ultra_Dynamic_Sky.Ultra_Dynamic_Sky_C|GetTime%20of%20Day _returnvalue) 5e+01))))))

(event Custom|Server%20Activate%20Crisis%20Ability
  (params (ID :type Integer) (Days :type Integer%20%28by%20ref%29) (Gold :type Integer))
  (bind _returnvalue (CallFunction|GetCrisisAbilityComponent))
  (Default|SetCooldownforAbility _returnvalue ID Days)
  (switch int ID ; 0 = Reduce\n1 = Reroll\n2 = Freeze
    (:0
      (bind _returnvalue_2 (CallFunction|GetCrisisComponents))
      (for _array_element _returnvalue_2
        (Default|EditDoom _array_element -2)))
    (:1
      (bind _returnvalue_3 (CallFunction|GetCrisisComponents))
      (for _array_element_2 _returnvalue_3
        (for (_ _array_index) (Variables|/Game/Blueprints/Crisis/BP_Crisis_Component.BP_Crisis_Component_C|GetMissions _array_element_2)
          (Default|RerollMission _array_element_2 _array_index))))
    (:2
      (bind _returnvalue_4 (CallFunction|GetCrisisComponents))
      (for _array_element_3 _returnvalue_4
        (Default|AddDaystoAllMissions _array_element_3 2)))))

(event Custom|Switch%20Lighting%20Layer
  (Utilities|FlowControl|FlipFlop
    (:A
      (Game|UnloadStreamLevel(byName) "UltraRandom" true)
      (Game|LoadStreamLevel(byName) "SyntyLighting5" true true))
    (:B
      (Game|UnloadStreamLevel(byName) "SyntyLighting5" true)
      (Game|LoadStreamLevel(byName) "UltraRandom" true true))))

(event Custom|Server%20Fund%20District
  (params (District :type Byte) (Coins :type Integer))
  (bind _returnvalue (CallFunction|GetCrisisComponentbyDistrictID District))
  (Default|EditRequiredCoins _returnvalue Coins))

(event Custom|Server%20Repossess
  (Pawn|Possess (Pawn|GetControlledPawn)))

(event Custom|Set%20Dungeon%20Ready
  (params (Dungeon%20Ready :type Boolean))
  (bind _returnvalue (Pawn|GetControlledPawn))
  (Variables|Default|SetDungeon%20Ready Dungeon%20Ready)
  (Utilities|FlowControl|Sequence
    (:then_0
      (Utilities|IsValid _returnvalue
        (:Is%20Valid
          (Actor|DestroyActor _returnvalue))))
    (:then_1
      (Class|GameModeBase|RestartPlayer (Game|GetGameMode) self))))

(event Custom|Server%20Reset%20Player%20Position
  ;[1 1 1] RPC to server to reset my position
  (CallFunction|ResetPlayerPosition))

(event Input|EnhancedActionEvents|EnhancedInputActionIA_Voice
  (params (ActionValue :type Boolean) (ElapsedSeconds :type Float%20%28double-precision%29) (TriggeredSeconds :type Float%20%28double-precision%29) (InputAction :type Input%20Action%20Object%20Reference :default "/Game/Blueprints/Input/IA_Voice.IA_Voice"))
  (:Started
    (CallFunction|SetChatting true))
  (:Canceled
    (CallFunction|SetChatting false :!label _label))
  (:Completed
    (goto _label)))

(event Input|EnhancedActionEvents|EnhancedInputActionIA_GameMaster
  (params (ActionValue :type Boolean) (ElapsedSeconds :type Float%20%28double-precision%29) (TriggeredSeconds :type Float%20%28double-precision%29) (InputAction :type Input%20Action%20Object%20Reference :default "/Game/Blueprints/Input/IA_GameMaster.IA_GameMaster"))
  ;[1 1 1] Enter/Exit
  (:Started
    (bind _foundwidgets (Widget|GetAllWidgetsOfClass "/Game/PCG/DungeonArchitect/W_LoadingDungeon.W_LoadingDungeon_C" true))
    (if (Utilities|Array|IsEmpty _foundwidgets)
      (bind _isa (Utilities|FlowControl|FlipFlop)
        (:A
          _)
        (:B
          _))
      (CallFunction|ToggleAdminCamera _isa))))

(event EventPossess
  (params (PossessedPawn :type Pawn%20Object%20Reference))
  (Game|AssignOnDestroyed PossessedPawn (delegate Custom|OnDestroyed_Event)))

(event EventBeginPlay
  (|CallParentFunction)
  (Networking|SwitchHasAuthority
    (:Authority
      (bind _returnvalue (Utilities|Time|SetTimerbyEvent (delegate Custom|Check%20for%20Pawn) 1.0 true))
      (Variables|Default|SetPawn%20Check _returnvalue))))

(event Input|KeyboardEvents|DebugKeyUp
  (params (Key :type Key%20Structure) (ActionValue :type Input%20Action%20Value%20Structure))
  (:Pressed
    (CallFunction|ServerChangeTime)))

(event Input|KeyboardEvents|DebugKeyDown
  (params (Key :type Key%20Structure) (ActionValue :type Input%20Action%20Value%20Structure))
  (:Pressed
    (CallFunction|ServerChangeWeather)))

(event Input|KeyboardEvents|DebugKeyRight
  (params (Key :type Key%20Structure) (ActionValue :type Input%20Action%20Value%20Structure))
  (:Pressed
    (CallFunction|SwitchLightingLayer)))

(fn ConstructionScript)

(fn FundDistrict
  (params (In%20District :type Byte) (In%20Funds :type Integer)))

(fn OnRepDungeonReady
  (Default|CallOnDungeonReady))

(fn ResetPlayerPosition
  (bind _returnvalue (Pawn|GetControlledPawn))
  (bind _l_debug (LocalVariables|GetL%20Debug))
  (bind _l_debug_2 (LocalVariables|GetL%20Debug))
  ;[1 1 1] This function finds a location around the player on the nav mesh
  ; if that fails, it grows the search radius
  ; once a navigation location is found, we test a path to any spawn point
  ; if we find a navigation location with a path to a spawn point, we move there
  ; because that means were not teleporting to navigation that is out of bounds
  (Utilities|FlowControl|ForLoopwithBreak 0 50 :!label _label
    (:LoopBody
      (bind _outactors (Actor|GetAllActorsOfClass "/Script/Engine.PlayerStart"))
      (LocalVariables|SetL%20Spawn (.OutItem (Utilities|Array|Random _outactors))) ; try different spawns
      (LocalVariables|SetL%20Radius (+ (LocalVariables|GetL%20Radius) 5e+02))
      (bind _randomlocation (Class|NavigationSystemV1|GetRandomLocationinNavigableRadius (Transformation|GetActorLocation (Pawn|GetControlledPawn)) (LocalVariables|GetL%20Radius) 0 0))
      (LocalVariables|SetL%20Location _randomlocation)
      (bind _returnvalue_2 (Class|NavigationSystemV1|FindPathtoLocationSynchronously (LocalVariables|GetL%20Location) (Transformation|GetActorLocation (LocalVariables|GetL%20Spawn)) (Pawn|GetControlledPawn) 0))
      (Utilities|IsValid _returnvalue_2
        (:Is%20Valid
          (Development|PrintString (Class|NavigationPath|GetDebugString _returnvalue_2) _l_debug_2 _l_debug_2)
          (if (and (not (Class|NavigationPath|IsPartial _returnvalue_2)) (Utilities|IsValid _returnvalue_2))
            (Transformation|Teleport _returnvalue (LocalVariables|GetL%20Location) (Transformation|GetActorRotation _returnvalue))
            (goto _label Break)))
        (:Is%20Not%20Valid
          (Development|PrintString "NO PATH" _l_debug _l_debug))))))