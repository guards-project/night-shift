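; Base HUD Blueprint that creates the player's main widget stack and, when a dungeon manager exists, a dungeon loading screen.
; BeginPlay clears widgets, waits briefly, then retries until a player controller is valid before building the UI.
; A looping watchdog timer recreates, re-adds or unhides the stack until it is visible, then stops.
; Helpers for the one-time hub menu with splash and a hidden escape menu go uncalled here.
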(event Custom|Check%20for%20HUD
  (Utilities|IsValid self
    (:Is%20Valid
      (bind _foundwidgets (Widget|GetAllWidgetsOfClass "/Game/_Guards/UserInterface/Menus/Stack/W_Stack_HUD.W_Stack_HUD_C" true))
      (if (Utilities|Array|IsEmpty _foundwidgets)
        (CallFunction|CreateHUDStack)
        (elif (UserInterface|Viewport|IsinViewport (Utilities|Array|Get(acopy) _foundwidgets))
          (if (Widget|IsVisible (Utilities|Array|Get(acopy) _foundwidgets))
            (Utilities|Time|ClearandInvalidateTimerbyHandle (Variables|Default|GetHUD%20Handle))
            (else
              (Widget|SetVisibility (Utilities|Array|Get(acopy) _foundwidgets) "Visible")))
          (else
            (UserInterface|Viewport|AddtoViewport (Utilities|Array|Get(acopy) _foundwidgets) 0)))))))

(event Custom|Start%20HUD%20Checks
  (bind _returnvalue (Utilities|Time|SetTimerbyEvent (delegate Custom|Check%20for%20HUD) 1.0 true))
  (Variables|Default|SetHUD%20Handle _returnvalue))

(event Custom|Start%20HUD
  (Utilities|IsValid (Game|GetPlayerController 0)
    (:Is%20Valid
      (CallFunction|CreateHUDStack)
      (CallFunction|CreateDungeonLoadingScreen)
      (Class|WidgetBlueprintLibrary|SetFocustoGameViewport))
    (:Is%20Not%20Valid
      (Utilities|FlowControl|Delay 0.2)
      (CallFunction|StartHUD))))

(event EventEndPlay
  (params (EndPlayReason :type EEndPlayReason%20Enum :default "Destroyed"))
  (Viewport|RemoveAllWidgets))

(event EventBeginPlay
  (Viewport|RemoveAllWidgets)
  (Utilities|FlowControl|Delay 1.0)
  (CallFunction|StartHUD))

(fn ConstructionScript)

(fn CreateDungeonLoadingScreen
  (bind _returnvalue (Actor|GetActorOfClass "/Game/PCG/DungeonArchitect/BP_Dungeon_Manager.BP_Dungeon_Manager_C"))
  (Utilities|IsValid _returnvalue
    (:Is%20Valid
      (bind _returnvalue_2 (UserInterface|CreateWidget "/Game/PCG/DungeonArchitect/W_LoadingDungeon.W_LoadingDungeon_C" (Game|Player|GetOwningPlayerController) _returnvalue))
      (UserInterface|Viewport|AddtoViewport _returnvalue_2 999))))

(fn CreateMenu
  (bind _returnvalue (Game|GetCurrentLevelName true))
  (if (and (Utilities|Enum|Equal(Enum) _returnvalue (Utilities|String|ToString(Name) (CallFunction|GetHUBWorld))) (not (Variables|/Game/Blueprints/Core/BP_GameInstance_Template.BP_GameInstance_Template_C|GetMenu%20Created (.AsBP%20Game%20Instance%20Template (Utilities|Casting|CastToBP_GameInstance_Template (Game|GetGameInstance))))))
    (bind _returnvalue_2 (UserInterface|CreateWidget "/Game/_Guards/UserInterface/Menus/MainMenu/W_MainMenu.W_MainMenu_C" (Game|Player|GetOwningPlayerController)))
    (UserInterface|Viewport|AddtoViewport _returnvalue_2 9990)
    (Variables|/Game/Blueprints/Core/BP_GameInstance_Template.BP_GameInstance_Template_C|SetMenu%20Created (.AsBP%20Game%20Instance%20Template (Utilities|Casting|CastToBP_GameInstance_Template (Game|GetGameInstance))) true)
    (bind _returnvalue_3 (UserInterface|CreateWidget "/Game/_Guards/UserInterface/Menus/MainMenu/W_Splash.W_Splash_C" (Game|Player|GetOwningPlayerController) _returnvalue_2))
    (UserInterface|Viewport|AddtoViewport _returnvalue_3 9991)))

(fn CreateEscapeScreen
  (bind _returnvalue (UserInterface|CreateWidget "/Game/_Guards/UserInterface/Menus/EscapeMenu/W_EscapeMenu.W_EscapeMenu_C"))
  (UserInterface|Viewport|AddtoViewport _returnvalue 1)
  (Widget|SetVisibility _returnvalue "Collapsed"))

(fn CreateHUDStack
  (bind _foundwidgets (Widget|GetAllWidgetsOfClass "/Game/_Guards/UserInterface/Menus/Stack/W_Stack_HUD.W_Stack_HUD_C" true))
  (for _array_element _foundwidgets
    (Utilities|IsValid _array_element
      (:Is%20Valid
        (Widget|RemovefromParent _array_element))))
  (bind _returnvalue (UserInterface|CreateWidget "/Game/_Guards/UserInterface/Menus/Stack/W_Stack_HUD.W_Stack_HUD_C" (Game|GetPlayerController 0)))
  (bind _output_get (Variables|Default|SetStack _returnvalue))
  (UserInterface|Viewport|AddtoViewport _output_get 0)
  (CallFunction|StartHUDChecks))

(fn GetWidgetStack
  (return (Variables|Default|GetStack)))