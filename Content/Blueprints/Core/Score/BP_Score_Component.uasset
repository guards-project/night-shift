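; Score component that keeps replicated per-player tallies of named score keys, stored by player name so they survive players leaving before round end.
; The server binds to the game mode's join callback, retrying until it exists, and seeds each player with zeroed keys from a data table.
; AddScore accumulates values on authority, GetScoreMap returns one player's or combined team totals, and OnRep broadcasts score updates.
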(event `self.ReceiveBeginPlay`
  (`/Engine/EditorBlueprintResources/ActorComponentMacros.Switch Has Authority`
    (:`Authority`
      (`self.Bind to Player States`))))

(event `Bind to Player States`
  (bind _returnvalue (`Actor.GetComponentByClass` (`GameplayStatics.GetGameMode`) "/Game/Blueprints/Core/Components/BP_PlayerJoinLeaveCallback.BP_PlayerJoinLeaveCallback_C"))
  (`/Engine/EditorBlueprintResources/StandardMacros.IsValid` _returnvalue
    (:`Is Valid`
      (add `/Game/Blueprints/Core/Components/BP_PlayerJoinLeaveCallback.Player Joined` _returnvalue (`|CreateDelegate` :!event `On Player Join`))
      (for _array_element (`GameStateBase.PlayerArray` (`GameplayStatics.GetGameState`))
        (bind _ascontroller (cast `Controller` (`Actor.GetOwner` _array_element)))
        (`self.On Player Join` _ascontroller (`Controller.PlayerState` _ascontroller))))
    (:`Is Not Valid`
      (`KismetSystemLibrary.K2_SetTimerDelegate` (delegate `Bind to Player States`) 0.5))))

(event `On Player Join`
  (params (Controller :type "Controller Object Reference") (PlayerState :type "PlayerState Object Reference"))
  (`self.Init Default Scores` (`PlayerState.GetPlayerName` PlayerState)))

(fn `Add Score`
  (params (`In Player Name` :type String) (`In Score Key` :type String) (`In Score` :type Integer))
  (locals (`L Score` :type "/Game/Blueprints/Core/Score/F_Score Structure") (`L Index` :type Integer) (`L Score Index` :type Integer :default 0))
  (bind ((`PlayerName_10_D260A7DB4FD0523E40D1FCA49FBA0138` _playername) (`ScoreTitle_17_A875D36F40BCA3BBE4A577A06BA11467` _scoretitle)) (break `/Game/Blueprints/Core/Score/F_Score` (`local.L Score`)))
  (bind ((`ScoreTitle_17_A875D36F40BCA3BBE4A577A06BA11467` _scoretitle_2) (`ScoreAmount_20_85B42D5F4803575A0D0DFC90762BEA04` _scoreamount)) (break `/Game/Blueprints/Core/Score/F_Score` (`local.L Score`)))
  (`/Engine/EditorBlueprintResources/ActorComponentMacros.Switch Has Authority`
    (:`Authority`
      (for (_array_element _array_index) (`self.Scores`)
        (set `local.L Score` _array_element)
        (set `local.L Index` _array_index)
        ;[1 1 1] Find existing player and update them
        (if (`KismetStringLibrary.EqualEqual_StrStr` (`local.In Player Name`) _playername)
          (set `local.L Score Index` (`KismetArrayLibrary.Array_Find` _scoretitle (`local.In Score Key`)))
          (if (>= (`local.L Score Index`) 0)
            (`KismetArrayLibrary.Array_Set` (`.ScoreAmount_20_85B42D5F4803575A0D0DFC90762BEA04` (break `/Game/Blueprints/Core/Score/F_Score` (`local.L Score`))) (`local.L Score Index`) (+ (`|GetArrayItem` (`.ScoreAmount_20_85B42D5F4803575A0D0DFC90762BEA04` (break `/Game/Blueprints/Core/Score/F_Score` (`local.L Score`))) (`local.L Score Index`)) (`local.In Score`)))
            (`KismetArrayLibrary.Array_Set` (`.ScoreTitle_17_A875D36F40BCA3BBE4A577A06BA11467` (break `/Game/Blueprints/Core/Score/F_Score` (`local.L Score`))) (`local.L Score Index`) (`local.In Score Key`))
            (else
              (`KismetArrayLibrary.Array_AddUnique` _scoretitle_2 (`local.In Score Key`))
              (bind _returnvalue (`KismetArrayLibrary.Array_Add` _scoreamount (`local.In Score`)))
              (set `local.L Score Index` _returnvalue)))
          (`KismetArrayLibrary.Array_Set` (`self.Scores`) (`local.L Index`) (`local.L Score`) true)
          (`KismetSystemLibrary.PrintString` (`KismetStringLibrary.Concat_StrStr` (`local.In Player Name`) " " (`local.In Score Key`) " = " (`KismetStringLibrary.Conv_IntToString` (`|GetArrayItem` (`.ScoreAmount_20_85B42D5F4803575A0D0DFC90762BEA04` (break `/Game/Blueprints/Core/Score/F_Score` (`local.L Score`))) (`local.L Score Index`))) " Updated"))
          (return)))
      ;[1 1 1] Add new player
      (`KismetArrayLibrary.Array_Add` (`self.Scores`) (make `/Game/Blueprints/Core/Score/F_Score` (`local.In Player Name`) (`|MakeArray` (`local.In Score Key`)) (`|MakeArray` (`local.In Score`))))
      (`KismetSystemLibrary.PrintString` (`KismetStringLibrary.Concat_StrStr` (`local.In Player Name`) " " (`local.In Score Key`) " = " (`KismetStringLibrary.Conv_IntToString` (`local.In Score`)) " New")))))

(fn `Get Score Map`
  (params (`In Player Name` :type String))
  (returns (`Score Amount` :type "Map of String to Integer"))
  (locals (`L Map` :type "Map of String to Integer") (`L Score` :type "/Game/Blueprints/Core/Score/F_Score Structure"))
  (bind _in_player_name (`local.In Player Name`))
  (bind (_playername _scoretitle _scoreamount) (break `/Game/Blueprints/Core/Score/F_Score` (`local.L Score`)))
  (for _array_element (`self.Scores`)
    (bind _output_get (set `local.L Score` _array_element))
    (if (or (`KismetStringLibrary.EqualEqual_StrStr` (`.PlayerName_10_D260A7DB4FD0523E40D1FCA49FBA0138` (break `/Game/Blueprints/Core/Score/F_Score` _output_get)) _in_player_name) (`KismetStringLibrary.IsEmpty` _in_player_name))
      ;[1 1 1] Add score to the map if it matches the in player name, or if the player was empty (tally all scores)
      ; If the key map find score key fails, it will return 0, added to the found score and enters the first entry of that key
      (for (_array_element_2 _array_index) _scoretitle
        (`BlueprintMapLibrary.Map_Add` (`local.L Map`) _array_element_2 (+ (`BlueprintMapLibrary.Map_Find` (`local.L Map`) _array_element_2) (`|GetArrayItem` _scoreamount _array_index))))
      ;[1 1 1] Return only the found player name mapped scores
      (if (not (`KismetStringLibrary.IsEmpty` (`local.In Player Name`)))
        (return (`local.L Map`)))))
  ;[1 1 1] Return all scores (team)
  (return (`local.L Map`)))

(fn `Init Default Scores`
  (params (`Player Name` :type String))
  (bind _default_score_keys (`self.Default Score Keys`))
  ;[1 1 1] This is neccesary otherwise the end round screen only shows what was logged,
  ; instead of 0 throws for example
  (bind _outrownames (`DataTableFunctionLibrary.GetDataTableRowNames` _default_score_keys))
  (for _array_element _outrownames
    (bind _returnvalue (`|GetDataTableRow` _default_score_keys _array_element)
      (:`then`
        (`self.Add Score` (`local.Player Name`) (`.Name_5_B1E5A0A8468F7014066943935A36837F` (break `/Game/Blueprints/Core/Score/F_ScoreData` _returnvalue))))))
  (return))

(fn `OnRep_Scores`
  (`self.Score Updated`))

(fn `Reset`
  (`KismetArrayLibrary.Array_Clear` (`self.Scores`))
  (set `self.Scores` (`self.Scores`)) ; update rep
)