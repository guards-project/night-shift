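; BP_PolygonAiArray is an actor that spawns a line-up of Polygon AI characters, one for each row of a data table.
; Its CreateAI event first destroys existing BP_Polygon_AI actors in the world, then loops over the table's row names.
; Each new AI takes the actor's rotation, is offset along world Y at even spacing and slightly raised, and receives its row handle as Config.
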(event `Create AI`
  (bind _outactors (`GameplayStatics.GetAllActorsOfClass` "/Game/Blueprints/Core/PolygonAI/BP_Polygon_AI.BP_Polygon_AI_C"))
  (`self.K2_DestroyActor` _outactors)
  (bind _outrownames (`DataTableFunctionLibrary.GetDataTableRowNames` (`self.Table`)))
  (for (_array_element _array_index) _outrownames
    (`|SpawnActorFromClass` "/Game/Blueprints/Core/PolygonAI/BP_Polygon_AI.BP_Polygon_AI_C" (`KismetMathLibrary.MakeTransform` (+ (`self.K2_GetActorLocation`) (`KismetMathLibrary.MakeVector` 0.0 (* _array_index 125.0) 90.0)) (`self.K2_GetActorRotation`)) "Undefined" "MultiplyWithRoot" null null (make `DataTableRowHandle` (`self.Table`) _array_element) null)))

(fn `UserConstructionScript`)