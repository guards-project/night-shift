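; Polygon AI character Blueprint for NPCs that players can arrest, rescue, revive or order to follow, with score and achievement tracking.
; A looping timer replaces Tick to update attack telegraphing and arrest montages, while replicated states drive targeting, collision and battle cries.
; Damage briefly slows free characters but makes arrested ones hurry.
; Death or arrest can drop coins, and sleeping dead ragdolls become pose-snapshot actors before the character is destroyed.
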(event `self.ReceiveBeginPlay`
  ;[0.3755 1 0.03063] Init
  (`parent.ReceiveBeginPlay`)
  (`self.On Arrested Changed`)
  (`self.Set Update Interval Active` true))

(event `Set Update Interval Active`
  (params (Condition :type Boolean))
  ;[1 1 1] optimisation
  (if Condition
    (bind _returnvalue (`KismetSystemLibrary.K2_SetTimerDelegate` (`|CreateDelegate` :!event `Update`) (`self.Update Interval`) true))
    (set `self.Update Handle` _returnvalue)
    (else
      (`KismetSystemLibrary.K2_ClearAndInvalidateTimerHandle` (`self.Update Handle`)))))

(event `Try Spawn Death Loot`
  ;[1 1 1] Death Loot
  (if (`self.Can Spawn Loot On Death`)
    (`/Engine/EditorBlueprintResources/StandardMacros.DoOnce` false
      (:`Completed`
        (`/Game/Blueprints/LootSpawner/BP_LootSpawner_Component.Spawn Loot` (`self.BP_LootSpawner_Component_Coins`) (+ (`SceneComponent.K2_GetComponentLocation` (`self.Mesh`)) (0.0 0.0 100.0)))))))

(event `Update`
  ;[1 0 0.01785] Tick
  (`self.Update Telegraphing`)
  (`self.Update Arrested`))

(event `self.On Death`
  ;[1 1 1] Death
  (`parent.On Death`)
  (`MeshComponent.SetScalarParameterValueOnMaterials` (`self.Mesh`) "Desaturation" 1.0)
  (`self.Set Update Interval Active` false)
  (`self.Try Spawn Death Loot`)
  (set `SkinnedMeshComponent.VisibilityBasedAnimTickOption` "AlwaysTickPoseAndRefreshBones" (`self.Mesh`)) ; required so snapshot isn't static pose
)

(event `self.Mesh.OnComponentSleep`
  (params (SleepingComponent :type "PrimitiveComponent Object Reference") (BoneName :type Name))
  ;[1 1 1] Wait for all bones to sleep, then create a snapshot actor that snapshots the pose
  (`/Engine/EditorBlueprintResources/ActorMacros.Switch Has Authority`
    (:`Authority`
      (bind _constraints (`self.Get Constraints`))
      (if (`KismetArrayLibrary.Array_IsEmpty` _constraints)
        (bind _dead (`/Game/Blueprints/Core/BPI_Character.Is Dead`))
        (if _dead
          (`/Engine/EditorBlueprintResources/StandardMacros.DoOnce` false
            (:`Completed`
              (`|ExecutionSequence`
                (:`then_0`
                  (`self.MC Snapshot`) ; fallback
                )
                (:`then_1`
                  (`/Engine/EditorBlueprintResources/ActorMacros.Switch Has Authority`
                    (:`Authority`
                      (`KismetSystemLibrary.Delay` 4.0) ; So that clients have time for the MC to land (or for the sleep to occur if client auth)
                      (`self.K2_DestroyActor`))))))))))))

(event `self.On Recovered`
  ;[1 1 1] Death
  (`parent.On Recovered`)
  (`MeshComponent.SetScalarParameterValueOnMaterials` (`self.Mesh`) "Desaturation" 0.0 :!label _label)
  (`self.Set Update Interval Active` true)
  (`self.Reset Miff Attack Ach`))

(event `self.On KO`
  ;[1 1 1] Death
  (`parent.On KO`)
  (`self.Set Update Interval Active` false))

(event `self.On Revived`
  ;[1 1 1] Death
  (`parent.On Revived`)
  (goto _label))

(event `MC Snapshot`
  (bind _mesh (`self.Mesh`))
  (bind _mesh_2 (`self.Mesh`))
  (bind _snapshot (`self.Snapshot`))
  (bind _returnvalue (`SkeletalMeshComponent.GetAnimInstance` _mesh))
  ;[1 1 1] Wait for all bones to sleep, then create a snapshot actor that snapshots the pose
  (`/Engine/EditorBlueprintResources/StandardMacros.Can Execute Cosmetic Events` :!label _label_2
    (:`True`
      (`/Engine/EditorBlueprintResources/StandardMacros.DoOnce` false
        (:`Completed`
          (`AnimInstance.SnapshotPose` _returnvalue _snapshot)
          (`|SpawnActorFromClass` "/Game/Blueprints/Core/PolygonAI/BP_SnapshotPose.BP_SnapshotPose_C" (`SceneComponent.K2_GetComponentToWorld` _mesh) "AlwaysSpawn" "MultiplyWithRoot" null _returnvalue _snapshot (`SkeletalMeshComponent.GetSkeletalMeshAsset` _mesh_2) (`PrimitiveComponent.GetMaterial` _mesh_2 0) null)
          (`self.SetActorHiddenInGame` true))))))

(event `Create Snapshot`
  ;[1 1 1] Wait for all bones to sleep, then create a snapshot actor that snapshots the pose
  (goto _label_2))

(event `On Arrested Changed`
  (bind _bp_team_component (`self.BP_Team_Component`))
  ;[1 1 1] On Arrested Changed Stop getting attacked and stop attacking enemies, and spawn loot
  (if (`self.Arrested`)
    (`self.Cleanup VFX`)
    (`self.Set Can Walk Through` true)
    (`/Engine/EditorBlueprintResources/ActorMacros.Switch Has Authority`
      (:`Authority`
        (set `self.Path Node` null)
        (set `/Game/Blueprints/Core/Components/BP_Team_Component.Can Target Enemies` false _bp_team_component)
        (set `/Game/Blueprints/Core/Components/BP_Team_Component.Can Be Targetted` false _bp_team_component)
        (`self.Auth Set Can Move` true)
        (`/Engine/EditorBlueprintResources/StandardMacros.DoOnce` false
          (:`Completed`
            (if (`self.Can Spawn Loot When Arrested`)
              (`/Game/Blueprints/LootSpawner/BP_LootSpawner_Component.Spawn Loot` (`self.BP_LootSpawner_Component_Coins`) (+ (`SceneComponent.K2_GetComponentLocation` (`self.Mesh`)) (0.0 0.0 20.0))))))))
    (else
      (`self.Set Can Walk Through` false)
      (`self.StopAnimMontage` (`self.Arrest Montage Stand`))
      (`self.StopAnimMontage` (`self.Arrest Montage Kneel`))
      (set `/Game/Blueprints/Core/Components/BP_Team_Component.Can Be Targetted` true (`self.BP_Team_Component`)))))

(event `self.BP_Health_Component.Health Changed`
  (params (Component :type "/Game/Blueprints/Core/Components/BP_Health_Component Object Reference") (Delta :type "Float (double-precision)") (`New Health` :type "Float (double-precision)") (`Damage Type` :type "DamageType Object Reference"))
  ;[1 1 1] When taking damage walk for 1 (slow down)
  ; If arrested, run faster (MOVE DAMMIT!)
  (`self.On Health Changed` Delta))

(event `Speed Up Arrest`
  ;[1 1 1] Punch to run faster
  (bind _returnvalue (`KismetSystemLibrary.K2_SetTimerDelegate` (delegate `Run Fast`) 0.5))
  (set `self.Run Fast Handle` _returnvalue))

(event `Run Fast`
  ;[1 1 1] Punch to run faster
  (bind _ko (`/Game/Blueprints/Core/BPI_Character.Is KO`))
  (bind _dead (`/Game/Blueprints/Core/BPI_Character.Is Dead`))
  (if (not (or _dead _ko))
    (`self.MC Stop Stagger`)
    (`AbilitySystemComponent.RemoveActiveEffectsWithTags` (`self.GSCAbilitySystem`) (struct :`GameplayTags` (struct :`(TagName` "Status.Stunned") :`(TagName` "Status.Stagger"))))
    (`self.Set Physical Animation` true)
    (`self.Auth Set Move State` (select `bool` (`self.Following`) :`false` "NewEnumerator1" :`true` "NewEnumerator2" :!type "/Game/Blueprints/Core/E_MoveState Enum"))
    (bind _returnvalue (`KismetSystemLibrary.K2_SetTimerDelegate` (delegate `Return to Desired Speed`) (`KismetMathLibrary.RandomFloatInRange` 3.0 4.0)))
    (set `self.Run Fast Handle` _returnvalue)))

(event `On Health Changed`
  (params (Delta :type "Float (double-precision)"))
  (bind _returnvalue (`AIBlueprintHelperLibrary.GetBlackboard` null))
  ;[1 1 1] When taking damage walk for 1 (slow down)
  ; If arrested, run faster (MOVE DAMMIT!)
  (if (< Delta 0.0)
    (if (`self.Arrested`)
      (`self.Speed Up Arrest`)
      (else
        (`/Game/Blueprints/Core/BPI_Character.Set Move State` "NewEnumerator0")
        (`KismetSystemLibrary.Delay` 1.0)
        (`/Engine/EditorBlueprintResources/StandardMacros.IsValid` _returnvalue
          (:`Is Valid`
            (`/Game/Blueprints/Core/BPI_Character.Set Move State` (`BlueprintMapLibrary.Map_Find` (`.MoveSetup_43_970037874107B618C5D7A7B3D444E862` (break `/Game/Blueprints/Core/PolygonAI/Config/F_Character_Setup` (`self.Config Data`))) (cast `/Game/Blueprints/Core/PolygonAI/Behaviour/E_AI_State` (`BlackboardComponent.GetValueAsEnum` _returnvalue "AI State")))))
          (:`Is Not Valid`
            (`/Game/Blueprints/Core/BPI_Character.Set Move State` "NewEnumerator1")))))))

(event `MC Stop Stars`
  ;[1 1 1] Punch to run faster
  (bind _niagara_stars (`self.Niagara Stars`)
    (:`then`
      (`ActorComponent.Deactivate` _niagara_stars)
      (`self.StopAnimMontage` (`self.Last Stun Montage`)))
    (:`else`)))

(event `MC Stop Stagger`
  ;[1 1 1] Punch to run faster
  (`self.StopAnimMontage` (`self.Last Stun Montage`)))

(event `Return to Desired Speed`
  ;[1 1 1] Punch to run faster
  (bind _ko (`/Game/Blueprints/Core/BPI_Character.Is KO`))
  (bind _dead (`/Game/Blueprints/Core/BPI_Character.Is Dead`))
  (if (not (or _dead _ko))
    (`self.Auth Set Move State` (select `bool` (`self.Following`) :`false` "NewEnumerator0" :`true` "NewEnumerator1" :!type "/Game/Blueprints/Core/E_MoveState Enum"))
    (`self.Set Physical Animation` false)
    (`self.MC Stop Stars`)))

(event `self.Score from Death`
  (params (`In Instigator` :type "Controller Object Reference"))
  ;[1 1 1] Remove arrest score if dead
  (`parent.Score from Death` `In Instigator`)
  (bind _arrester (`self.Arrester`)
    (:`then`
      (`/Game/Blueprints/Core/Score/BPFL_Score.Add Score` (`PlayerState.GetPlayerName` _arrester) "Arrests" -1))
    (:`else`)))

(event `Set Can Walk Through`
  (params (`Can Walk Through` :type Boolean))
  (`PrimitiveComponent.SetCollisionResponseToChannel` (`self.CapsuleComponent`) "ECC_Pawn" (select `bool` `Can Walk Through` :`false` "ECR_Block" :`true` "ECR_Ignore" :!type "ECollisionResponse Enum")))

(event `self.Play Getup`
  (bind _getup_montage (`self.Getup Montage`))
  ;[1 1 1] Getup overrides
  (`self.StopAnimMontage` _getup_montage)
  (bind _returnvalue (`self.PlayAnimMontage` _getup_montage))
  (`KismetSystemLibrary.Delay` (/ _returnvalue 1.8))
  (`self.Getup Complete`))

(event `self.Play Recover Sound`
  (`KismetSystemLibrary.Delay` 0.5)
  (if (not (`self.Arrested`))
    (`parent.Play Recover Sound`)))

(event `self.Getup Complete`
  ;[1 1 1] Getup overrides
  (`parent.Getup Complete`)
  (if (`self.Arrested`)
    (`self.Play Arrest Montage`)))

(event `/Game/Primer/Primer_Interaction/BPI_Interact.Execute Interact`
  (params (User :type "Controller Object Reference"))
  ;[1 1 1] Interact
  (`parent.Execute Interact` User)
  (`/Engine/EditorBlueprintResources/ActorMacros.Switch Has Authority`
    (:`Authority`
      (bind _dead (`/Game/Blueprints/Core/BPI_Character.Is Dead`))
      (if (not _dead)
        (bind _arrested (`self.Arrest` User))
        (if (not _arrested)
          (`self.Rescue` User)
          (`self.Set Following` User (or (not (`self.Following`)) (!= (`self.Leader`) (`Controller.K2_GetPawn` User)))))))))

(event `MC Arrest`
  (params (Controller :type "Controller Object Reference"))
  ;[1 1 1] Interact
  (`/Engine/EditorBlueprintResources/StandardMacros.Can Execute Cosmetic Events`
    (:`True`
      (`GameplayStatics.PlaySoundAtLocation` "/Game/Fantasy_Interface_SFX/cue/LockAndKey.LockAndKey" (`SceneComponent.K2_GetComponentLocation` (`self.Mesh`)) (struct) 1.0 1.0 0.0 "/Game/Blueprints/GAS/Cues/Sounds/ATT_Close.ATT_Close" null null null)
      (`/Engine/EditorBlueprintResources/StandardMacros.DoOnce` false
        (:`Completed`
          (`/Engine/EditorBlueprintResources/StandardMacros.IsValid` Controller
            (:`Is Valid`
              (if (`Controller.IsLocalPlayerController` Controller)
                (`self.Increment Arrests`)))))))))

(event `self.Set Last Zeroed By`
  (params (Instigator :type "Controller Object Reference"))
  (`parent.Set Last Zeroed By` Instigator)
  (`/Engine/EditorBlueprintResources/ActorMacros.Switch Has Authority`
    (:`Authority`
      (`|ExecutionSequence`
        (:`then_0`
          ;[1 1 1] Killed whilst miffed.
          (bind _last_zeroed_by (`self.Last Zeroed By`)
            (:`then`
              (if (`GSCBlueprintFunctionLibrary.HasMatchingGameplayTag` (`Controller.K2_GetPawn` _last_zeroed_by) (struct :`TagName` "Status.Miffed"))
                (bind _returnvalue (`self.GetComponentByClass` _last_zeroed_by "/Game/_Guards/OnlineSubsystem/Achievements/BP_Achievement_Component.BP_Achievement_Component_C"))
                (`/Engine/EditorBlueprintResources/StandardMacros.IsValid` _returnvalue
                  (:`Is Valid`
                    (`/Engine/EditorBlueprintResources/StandardMacros.DoOnce` false :!label _label_3
                      (:`Completed`
                        (`/Game/_Guards/OnlineSubsystem/Achievements/BP_Achievement_Component.Owner Write Achievement` _returnvalue "MiffAttack")))))))
            (:`else`)))
        (:`then_1`
          ;[1 1 1] Increment Player Kills
          (bind _dead (`/Game/Blueprints/Core/BPI_Character.Is Dead`))
          (if _dead
            (bind _last_zeroed_by_2 (`self.Last Zeroed By`)
              (:`then`
                (bind _returnvalue_2 (`self.GetComponentByClass` _last_zeroed_by_2 "/Game/_Guards/OnlineSubsystem/Achievements/BP_Achievement_Component.BP_Achievement_Component_C"))
                (`/Engine/EditorBlueprintResources/StandardMacros.IsValid` _returnvalue_2
                  (:`Is Valid`
                    (`/Game/_Guards/OnlineSubsystem/Achievements/BP_Achievement_Component.Owner Achievement Progress` _returnvalue_2 "Player_Kills" "Goal_Kill_500" 1))))
              (:`else`))))))))

(event `Reset Miff Attack Ach`
  ;[1 1 1] Killed whilst miffed.
  (goto _label_3 :!via `Reset`))

(event `Increment Arrests`
  ;[1 1 1] Increment Arrest count
  (`|SpawnActorFromClass` "/Game/_Guards/OnlineSubsystem/Achievements/BP_AchievementProgressor.BP_AchievementProgressor_C" (`KismetMathLibrary.Conv_VectorToTransform` (0.0 0.0 0.0)) "AlwaysSpawn" "MultiplyWithRoot" null "Player_Arrests" "Goal_Arrest_500" 1 null))

(event `self.Apply Character Config`
  ;[1 1 1] WIP
  (`parent.Apply Character Config`)
  (`/Engine/EditorBlueprintResources/ActorMacros.Switch Has Authority`))

(event `self.BP_Inventory_Component.OnEquippedItemChanged`
  (params (Mainhand :type "/Game/Blueprints/Items/BP_Item Object Reference") (Offhand :type "/Game/Blueprints/Items/BP_Item Object Reference"))
  (bind _returnvalue (`AIBlueprintHelperLibrary.GetBlackboard` null))
  (`/Engine/EditorBlueprintResources/StandardMacros.IsValid` Mainhand
    (:`Is Valid`
      (`/Engine/EditorBlueprintResources/StandardMacros.IsValid` _returnvalue
        (:`Is Valid`
          (`BlackboardComponent.SetValueAsFloat` _returnvalue "AttackRate" (`/Game/Blueprints/Items/BP_Item.AI Attack Rate` Mainhand)))))
    (:`Is Not Valid`
      (`/Engine/EditorBlueprintResources/StandardMacros.IsValid` _returnvalue
        (:`Is Valid`
          (`BlackboardComponent.SetValueAsFloat` _returnvalue "AttackRate" (`KismetMathLibrary.RandomFloatInRange` 0.4 0.7)))))))

(fn `Arrest`
  (params (`In Controller` :type "Controller Object Reference"))
  (returns (Arrested :type Boolean))
  (bind _in_controller (`local.In Controller`))
  ;[1 1 1] Arrest
  (if (and (`self.Can Arrest`) (not (`self.Arrested`)))
    (set `self.Arrested` true)
    (`self.MC Arrest` _in_controller)
    (bind _playerstate (`Controller.PlayerState` _in_controller)
      (:`then`
        (set `self.Arrester` _playerstate)
        (`/Game/Blueprints/Core/Score/BPFL_Score.Add Score` (`PlayerState.GetPlayerName` _playerstate) "Arrests" 1)
        (return true))
      (:`else`))
    (else
      (return false))))

(fn `Auth Set Can Move`
  (params (`Can Move` :type Boolean))
  ;[1 1 1] Stops anything setting can move to false after being arrested, which sets can move to true
  ; a race happens with GA_Throw for Thrower enemy which arrests and sets can move to true, but then sets it to false again permanently
  (if `Can Move`
    (`parent.Auth Set Can Move` `Can Move`)
    (elif (not (`self.Arrested`))
      (`parent.Auth Set Can Move` `Can Move`))))

(fn `Get Can Interact`
  (returns (ReturnValue :type Boolean))
  ;[1 1 1] Revive From Dead
  (bind _dead (`/Game/Blueprints/Core/BPI_Character.Is Dead`))
  (if _dead
    (return (`self.Can Revive from Dead`))
    (else
      ;[1 1 1] Arrest while KO
      (bind _ko (`/Game/Blueprints/Core/BPI_Character.Is KO`))
      (if _ko
        (if (`self.Can Arrest`)
          (return true)
          (else
            ;[1 1 1] Revive
            (return true)))
        (else
          ;[1 1 1] Rescue (ie unarrest)
          (if (and (`self.Arrested`) (`self.Can Rescue`))
            (return true)
            (else
              ;[1 1 1] Follow / Stay
              (if (`self.Can Follow`)
                (if (`self.Follow Requires Arrested`)
                  (return (`self.Arrested`))
                  (else
                    (return true)))))))))))

(fn `Get Interact Duration`
  (returns (Duration :type "Float (double-precision)"))
  (return 1.0))

(fn `Get Interact Text`
  (returns (Text :type Text))
  ;[1 1 1] Revive From Dead
  (bind _dead (`/Game/Blueprints/Core/BPI_Character.Is Dead`))
  (if _dead
    (if (`self.Can Arrest`)
      (return "Arrest")
      (else
        (return "Revive")))
    (else
      ;[1 1 1] Arrest while KO
      (bind _ko (`/Game/Blueprints/Core/BPI_Character.Is KO`))
      (if _ko
        (if (`self.Can Arrest`)
          (return "Arrest")
          (else
            ;[1 1 1] Revive
            (return "Revive")))
        (else
          ;[1 1 1] Rescue (ie unarrest)
          (if (and (`self.Arrested`) (`self.Can Rescue`))
            (return "Rescue")
            (else
              ;[1 1 1] Follow / Stay
              (return (select `bool` (and (`self.Following`) (== (`self.Leader`) (`Controller.K2_GetPawn` (`GameplayStatics.GetPlayerController` 0)))) :`false` "Follow" :`true` "Stay" :!type "Text")))))))))

(fn `Get Last Attack Hit`
  (returns (Hit :type Boolean))
  (return false))

(fn `Get Node Data`
  (returns (`Node Data` :type "/Game/Blueprints/Core/PolygonAI/PathNodes/F_PathNode Structure"))
  (return))

(fn `Get Path Node`
  (returns (`Path Node` :type "/Game/Blueprints/Core/PolygonAI/PathNodes/BP_PathNode Object Reference"))
  (return (`self.Path Node`)))

(fn `Init Attached Path`
  (bind _returnvalue (`self.GetAttachParentActor`))
  (`/Engine/EditorBlueprintResources/StandardMacros.IsValid` _returnvalue
    (:`Is Valid`
      (bind _asbp_path_node (cast `/Game/Blueprints/Core/PolygonAI/PathNodes/BP_PathNode` _returnvalue))
      (set `self.Path Node` _asbp_path_node))))

(fn `On Follow Changed`
  (`|ExecutionSequence`
    (:`then_0`
      (if (`self.Arrested`)
        (`self.Play Arrest Montage`)))
    (:`then_1`
      (if (`self.Following`)
        (`self.Set Can Walk Through` false)
        (else
          (`self.Set Can Walk Through` true))))))

(fn `OnRep_Arrested`
  (`self.On Arrested Changed`)
  (`self.On Arrested Updated` self (`self.Arrested`))
  (bind _getup_montage (`self.Getup Montage`)
    (:`then`
      (if (== _getup_montage (`AnimInstance.GetCurrentActiveMontage` (`SkeletalMeshComponent.GetAnimInstance` (`self.Mesh`))))
        (`self.Play Getup`) ; retrigger
      ))
    (:`else`)))

(fn `OnRep_Following`
  (`self.On Follow Changed`))

(fn `OnRep_Is Telegraphing`
  (if (`self.Is Telegraphing`)
    (`/Engine/EditorBlueprintResources/StandardMacros.Can Execute Cosmetic Events`
      (:`True`
        (`/Game/_Guards/Audio/VoiceSet/BP_Voice_Component.Play Voice` (`self.BP_Voice_Component`) "BattleCry")))))

(fn `Play Arrest Montage`
  (`self.PlayAnimMontage` (select `bool` (or (`self.Following`) (`KismetSystemLibrary.IsValid` (`self.Path Node`))) :`false` (`self.Arrest Montage Kneel`) :`true` (`self.Arrest Montage Stand`))))

(fn `Rescue`
  (params (`In Controller` :type "Controller Object Reference"))
  (returns (Success :type Boolean))
  ;[1 1 1] Rescue
  (if (and (`self.Can Rescue`) (`self.Arrested`))
    (set `self.Arrested` false)
    (bind _asai_controller_polygon (cast `/Game/Blueprints/Core/PolygonAI/Behaviour/AI_Controller_Polygon` (`AIBlueprintHelperLibrary.GetAIController` self)))
    ;[1 1 1] Hostages who are rescued cannot fight, only follow
    (`/Game/Blueprints/Core/PolygonAI/Behaviour/AI_Controller_Polygon.Set AI Senses Enabled` _asai_controller_polygon true)
    (bind _aiperception (`/Game/Blueprints/Core/PolygonAI/Behaviour/AI_Controller_Polygon.AIPerception` _asai_controller_polygon))
    (`AIPerceptionComponent.SetSenseEnabled` _aiperception "/Script/AIModule.AISense_Damage" false)
    (`AIPerceptionComponent.SetSenseEnabled` _aiperception "/Script/AIModule.AISense_Hearing" false)
    (`AIPerceptionComponent.SetSenseEnabled` _aiperception "/Script/AIModule.AISense_Sight" false)
    ;[1 1 1] Optional full retreat
    (if (`self.Should Retreat After Rescue`)
      (`/Game/Blueprints/Core/PolygonAI/Behaviour/AI_Controller_Polygon.Set BB AI State` _asai_controller_polygon "NewEnumerator4")
      (return true)
      (else
        (return true)))
    (else
      (return false))))

(fn `Set Following`
  (params (`In Controller` :type "Controller Object Reference") (`In Following` :type Boolean))
  (bind _returnvalue (`Controller.K2_GetPawn` (`local.In Controller`)))
  ;[1 1 1] On Interact Follow
  (if (`self.Can Follow`)
    (set `self.Following` (`local.In Following`))
    (if (`self.Following`)
      (bind _asai_controller_polygon (cast `/Game/Blueprints/Core/PolygonAI/Behaviour/AI_Controller_Polygon` (`AIBlueprintHelperLibrary.GetAIController` self)))
      (`/Game/Blueprints/Core/PolygonAI/Behaviour/AI_Controller_Polygon.Set BB FollowTarget` _asai_controller_polygon _returnvalue)
      (`/Game/Blueprints/Core/PolygonAI/Behaviour/AI_Controller_Polygon.Set BB AI State` _asai_controller_polygon "NewEnumerator5")
      (set `self.Leader` _returnvalue)
      (else
        (bind _asai_controller_polygon_2 (cast `/Game/Blueprints/Core/PolygonAI/Behaviour/AI_Controller_Polygon` (`AIBlueprintHelperLibrary.GetAIController` self)))
        (`/Game/Blueprints/Core/PolygonAI/Behaviour/AI_Controller_Polygon.Set BB FollowTarget` _asai_controller_polygon_2 null)
        (`/Game/Blueprints/Core/PolygonAI/Behaviour/AI_Controller_Polygon.Set BB AI State` _asai_controller_polygon_2 "NewEnumerator0")
        (set `self.Leader` null)))))

(fn `Should Telegraph Attack`
  (returns (Telegraph :type Boolean))
  (return (and (`self.Is Telegraphing`) (`self.Can Ever Telegraph Attack`))))

(fn `Update Arrested`
  (if (`self.Arrested`)
    (if (not (`AnimInstance.IsAnyMontagePlaying` (`SkeletalMeshComponent.GetAnimInstance` (`self.Mesh`))))
      (`self.Play Arrest Montage`))))

(fn `Update Telegraphing`
  (locals (`L Should Telegraph` :type Boolean))
  (bind _l_should_telegraph (`local.L Should Telegraph`))
  (`/Engine/EditorBlueprintResources/ActorMacros.Switch Has Authority`
    (:`Authority`
      (`/Engine/EditorBlueprintResources/StandardMacros.IsValid` (`self.GetController`)
        (:`Is Valid`
          (`|ExecutionSequence`
            (:`then_0`
              ;[1 1 1] onfigure should teelgraph
              (if (or (`GSCBlueprintFunctionLibrary.HasAnyMatchingGameplayTag` self (struct :`GameplayTags` (struct :`(TagName` "Status.Stunned") :`(TagName` "Status.Dead") :`(TagName` "Status.KO")))) (`self.Arrested`))
                (set `local.L Should Telegraph` false)
                (else
                  (bind _distance (message `/Game/Blueprints/Core/PolygonAI/Behaviour/BPI_AI.Get Distance to Target` (`self.GetController`)))
                  (set `local.L Should Telegraph` (and (> _distance 300.0) (<= _distance 750.0))))))
            (:`then_1`
              ;[1 1 1] Update telegraphing
              (if (!= _l_should_telegraph (`self.Is Telegraphing`))
                (set `self.Is Telegraphing` _l_should_telegraph)))))))))

(fn `UserConstructionScript`
  (`parent.UserConstructionScript`)
  (`self.Init Attached Path`))