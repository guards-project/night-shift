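; BP_SnapshotPose is an actor that shows a skeletal mesh frozen in a stored pose snapshot.
; The construction script applies the mesh and material, then passes the snapshot to ABP_Snapshot, the mesh's anim instance.
; Shortly after BeginPlay it makes the mesh visible, enables update rate optimizations and ticks the pose only when rendered to save animation cost.
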(event `self.ReceiveBeginPlay`
  (bind _skeletalmesh (`self.SkeletalMesh`))
  (`KismetSystemLibrary.Delay` 0.01)
  (`SceneComponent.SetVisibility` (`self.SkeletalMesh`) true false)
  (set `SkinnedMeshComponent.bEnableUpdateRateOptimizations` true _skeletalmesh)
  (set `SkinnedMeshComponent.VisibilityBasedAnimTickOption` "OnlyTickPoseWhenRendered" _skeletalmesh))

(fn `Apply Snapshot`
  (bind _skeletalmesh (`self.SkeletalMesh`)
    (:`then`
      (`SkeletalMeshComponent.SetSkeletalMeshAsset` _skeletalmesh (`self.Mesh`))
      (`PrimitiveComponent.SetMaterial` _skeletalmesh 0 (`self.Material`))
      (bind _asabp_snapshot (cast `/Game/Blueprints/Core/PolygonAI/ABP_Snapshot` (`SkeletalMeshComponent.GetAnimInstance` (`self.SkeletalMesh`))))
      (set `/Game/Blueprints/Core/PolygonAI/ABP_Snapshot.Snapshot` (`self.Snapshot`) _asabp_snapshot))
    (:`else`)))

(fn `UserConstructionScript`
  (`self.Apply Snapshot`))