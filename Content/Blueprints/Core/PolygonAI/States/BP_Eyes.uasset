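; BP_Eyes is an actor that places two Niagara eye effects on the head of its owning character.
; It snaps to the mesh's head socket with a fixed rotation offset, both on BeginPlay and when the replicated OwnerCharacter arrives.
; Where cosmetic events can run, it binds to a player character's third-person change event, hiding both effects from the owner outside third person.
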(event `self.ReceiveBeginPlay`
  (`self.Attach`))

(fn `Attach`
  (bind _owner_character (`self.Owner Character`)
    (:`then`
      (`self.K2_AttachToComponent` (`Character.Mesh` _owner_character) "head" "SnapToTarget" "SnapToTarget" "SnapToTarget")
      (`self.K2_SetActorRelativeRotation` (struct :`Pitch` 90.0 :`Yaw` 90.0))
      (`/Engine/EditorBlueprintResources/StandardMacros.Can Execute Cosmetic Events`
        (:`True`
          (bind _owner_character_2 (`self.Owner Character`)
            (:`then`
              (bind _asbp_character_template_player (cast `/Game/Blueprints/Core/BP_Character_Template_Player` _owner_character_2))
              (add `/Game/Blueprints/Core/BP_Character_Template_Player.Third Person Changed` _asbp_character_template_player (`|CreateDelegate` :!event `On Third Person Changed`)))
            (:`else`)))))
    (:`else`)))

(fn `On Third Person Changed`
  (params (`Is Third Person` :type Boolean))
  (`PrimitiveComponent.SetOwnerNoSee` (`|MakeArray` (`self.Niagara1`) (`self.Niagara`) :!type "PrimitiveComponent Object Reference") (not `Is Third Person`)))

(fn `OnRep_Owner Character`
  (`self.Attach`))

(fn `UserConstructionScript`)