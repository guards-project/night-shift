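; Civilian AI variant that drives its montage animations from follow, arrest and rescue state.
; Arrest updates and follow changes both run the same logic after calling the parent, leaving animation alone while arrested.
; Following civilians play a scared montage, which stops once they reach the APC safe zone; unrescued, unfollowed civilians kneel.
; It also sets a short interaction duration.
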(event `self.Update Arrested`
  ;[1 1 1] Update anim based on follow, arrest, or rescue
  ; Rescued comes from BP_FollowerAutoStop when the civilian reaches the safe zone
  (`parent.Update Arrested`)
  (if (`self.Arrested`) :!label _label
    _
    (elif (`self.Following`)
      ;[1 1 1] If following, not montaging, and should be scared, play scared
      (if (not (`AnimInstance.Montage_IsPlaying` (`SkeletalMeshComponent.GetAnimInstance` (`self.Mesh`)) "/Game/Polygon/Animations/PolygonAnims/Misc/AM_Scared.AM_Scared"))
        (`self.PlayAnimMontage` "/Game/Polygon/Animations/PolygonAnims/Misc/AM_Scared.AM_Scared"))
      (else
        ;[1 1 1] Stop Scared when rescued
        (if (`self.At APC`)
          (if (`AnimInstance.Montage_IsPlaying` (`SkeletalMeshComponent.GetAnimInstance` (`self.Mesh`)) "/Game/Polygon/Animations/PolygonAnims/Misc/AM_Scared.AM_Scared")
            (`AnimInstance.Montage_Stop` (`SkeletalMeshComponent.GetAnimInstance` (`self.Mesh`)) 0.0 "/Game/Polygon/Animations/PolygonAnims/Misc/AM_Scared.AM_Scared"))
          (else
            ;[1 1 1] if not following, not montaging, and not rescued (standing alone somewhere)
            ; Then kneel
            (if (not (`AnimInstance.Montage_IsPlaying` (`SkeletalMeshComponent.GetAnimInstance` (`self.Mesh`)) (`self.Arrest Montage Kneel`)))
              (`self.PlayAnimMontage` (`self.Arrest Montage Kneel`)))))))))

(event `self.On Follow Changed`
  (`parent.On Follow Changed`)
  (goto _label))

(fn `Get Interact Duration`
  (returns (Duration :type "Float (double-precision)"))
  (return 0.5))

(fn `UserConstructionScript`
  (`parent.UserConstructionScript`))