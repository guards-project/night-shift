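; Escort variant of the Polygon AI character that follows a path while a player stays inside its escort sphere.
; On the server it caches and clears its path at BeginPlay, then restores it after a short delay when the arrested state matches PathWhenArrested.
; Sphere overlaps, arrest changes and AI target changes re-evaluate movement, setting walk speed to zero when conditions fail.
; CanMoveWhileFree lets an unarrested escort move without players nearby.
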(event `self.ReceiveBeginPlay`
  (`|ExecutionSequence`
    (:`then_0`
      (`/Engine/EditorBlueprintResources/ActorMacros.Switch Has Authority`
        (:`Authority`
          (`self.Update Moving`)
          (`self.Bind to Target Changed`)
          (`self.Cache Path For Later`))))
    (:`then_1`
      (`parent.ReceiveBeginPlay`))))

(event `self.Sphere_Escort.OnComponentBeginOverlap`
  (params (OverlappedComponent :type "PrimitiveComponent Object Reference") (OtherActor :type "Actor Object Reference") (OtherComp :type "PrimitiveComponent Object Reference") (OtherBodyIndex :type Integer) (bFromSweep :type Boolean) (SweepResult :type "HitResult Structure (by ref)"))
  (`/Engine/EditorBlueprintResources/ActorMacros.Switch Has Authority`
    (:`Authority`
      (if (`self.ActorHasTag` OtherActor "Player")
        (`self.Update Moving`)))))

(event `self.On Arrested Changed`
  (bind _path_when_arrested (`self.Path When Arrested`))
  (`parent.On Arrested Changed`)
  (`/Engine/EditorBlueprintResources/ActorMacros.Switch Has Authority`
    (:`Authority`
      (`|ExecutionSequence`
        (:`then_0`
          (if (`self.Arrested`)
            (if _path_when_arrested
              (`KismetSystemLibrary.Delay` 0.2 :!label _label)
              (`self.Re-Init Path`))
            (elif (not _path_when_arrested)
              (goto _label))))
        (:`then_1`
          (`self.Update Moving`))))))

(event `Bind to Target Changed`
  (add `/Game/Blueprints/Core/PolygonAI/Behaviour/AI_Controller_Polygon.Target Changed` (cast `/Game/Blueprints/Core/PolygonAI/Behaviour/AI_Controller_Polygon` (`self.GetController`) :!pure true) (delegate `Target Changed_Event`)))

(event `self.Sphere_Escort.OnComponentEndOverlap`
  (params (OverlappedComponent :type "PrimitiveComponent Object Reference") (OtherActor :type "Actor Object Reference") (OtherComp :type "PrimitiveComponent Object Reference") (OtherBodyIndex :type Integer))
  (`/Engine/EditorBlueprintResources/ActorMacros.Switch Has Authority`
    (:`Authority`
      (if (`self.ActorHasTag` OtherActor "Player")
        (`self.Update Moving`)))))

(event `Target Changed_Event`
  (params (Controller :type "/Game/Blueprints/Core/PolygonAI/Behaviour/AI_Controller_Polygon Object Reference"))
  (`self.Update Move Speed`))

(event `Update Moving`
  (bind _returnvalue (and (not (`self.Arrested`)) (`self.Can Move While Free`)))
  (`self.Set Moving` (or (and (`KismetArrayLibrary.Array_IsValidIndex` (`PrimitiveComponent.GetOverlappingActors` (`self.Sphere_Escort`) "/Game/Blueprints/Core/BP_Character_Template_Player.BP_Character_Template_Player_C")) (or (and (`self.Path When Arrested`) (`self.Arrested`) (`KismetSystemLibrary.IsValid` (`self.Path Node`))) (and (not (`self.Path When Arrested`)) (not (`self.Arrested`)) (`KismetSystemLibrary.IsValid` (`self.Path Node`))) _returnvalue)) _returnvalue)) ; move if there are any overlapping players
)

(event `self.Update Move Speed`
  (`self.Update Moving`))

(event `Set Moving`
  (params (Moving :type Boolean))
  (if Moving
    (`parent.Update Move Speed`)
    (else
      (set `CharacterMovementComponent.MaxWalkSpeed` 0.0 (`self.CharacterMovement`)))))

(fn `Cache Path For Later`
  (set `self.Cached Path` (`self.Path Node`))
  (set `self.Path Node` null))

(fn `Get Path Node`
  (returns (`Path Node` :type "/Game/Blueprints/Core/PolygonAI/PathNodes/BP_PathNode Object Reference"))
  (if (`self.Arrested`)
    (bind _path_node (`parent.Get Path Node`))
    (return _path_node)
    (else
      (return null))))

(fn `Re-Init Path`
  (set `self.Path Node` (`self.Cached Path`))
  (bind _asai_controller_polygon (cast `/Game/Blueprints/Core/PolygonAI/Behaviour/AI_Controller_Polygon` (`self.GetController`)))
  (`/Game/Blueprints/Core/PolygonAI/Behaviour/AI_Controller_Polygon.Init Path` _asai_controller_polygon))

(fn `UserConstructionScript`
  (`parent.UserConstructionScript`))