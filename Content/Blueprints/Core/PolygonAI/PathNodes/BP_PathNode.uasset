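; Placeable PolygonAI path node that links to next and previous nodes to form a chain and exposes its node data.
; Its construction script clears self-links, fills empty reciprocal links on neighbours and labels the node with its name.
; It also refreshes its own and neighbours' splines to draw the link to each next node.
; GetAllLinkedPathNodes gathers the chain recursively in both directions, using AddUnique to stop on loops.
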(fn `Get All Linked Path Nodes`
  (returns (Nodes :type "Array of /Game/Blueprints/Core/PolygonAI/PathNodes/BP_PathNode Object Reference"))
  (locals (`L Nodes` :type "Array of /Game/Blueprints/Core/PolygonAI/PathNodes/BP_PathNode Object Reference"))
  (`KismetArrayLibrary.Array_Add` (`local.L Nodes`) self)
  (`|ExecutionSequence`
    (:`then_0`
      (bind _next_node (`self.Next Node`)
        (:`then`
          (bind _nodes (`self.Get Next Node Recursive` _next_node (`local.L Nodes`)))
          (`KismetArrayLibrary.Array_Append` (`local.L Nodes`) _nodes))
        (:`else`)))
    (:`then_1`
      (bind _previous_node (`self.Previous Node`)
        (:`then`
          (bind _nodes_2 (`self.Get Previous Node Recursive` _previous_node (`local.L Nodes`)))
          (`KismetArrayLibrary.Array_Append` (`local.L Nodes`) _nodes_2))
        (:`else`)))
    (:`then_2`
      (return (`local.L Nodes`)))))

(fn `Get Next Node Recursive`
  (params (`In Nodes` :type "Array of /Game/Blueprints/Core/PolygonAI/PathNodes/BP_PathNode Object Reference"))
  (returns (Nodes :type "Array of /Game/Blueprints/Core/PolygonAI/PathNodes/BP_PathNode Object Reference"))
  (locals (`L Nodes` :type "Array of /Game/Blueprints/Core/PolygonAI/PathNodes/BP_PathNode Object Reference"))
  (set `local.L Nodes` `In Nodes`)
  (bind _returnvalue (`KismetArrayLibrary.Array_AddUnique` (`local.L Nodes`) self))
  (if (>= _returnvalue 0)
    (`|ExecutionSequence`
      (:`then_0`
        (bind _next_node (`self.Next Node`)
          (:`then`
            (bind _nodes (`self.Get Next Node Recursive` _next_node (`local.L Nodes`)))
            (`KismetArrayLibrary.Array_Append` (`local.L Nodes`) _nodes))
          (:`else`)))
      (:`then_1`
        (return (`local.L Nodes`))))))

(fn `Get Node Data`
  (returns (`Node Data` :type "/Game/Blueprints/Core/PolygonAI/PathNodes/F_PathNode Structure"))
  (return (`self.Node Data`)))

(fn `Get Path Node`
  (returns (`Path Node` :type "/Game/Blueprints/Core/PolygonAI/PathNodes/BP_PathNode Object Reference"))
  (return null))

(fn `Get Previous Node Recursive`
  (params (`In Nodes` :type "Array of /Game/Blueprints/Core/PolygonAI/PathNodes/BP_PathNode Object Reference"))
  (returns (Nodes :type "Array of /Game/Blueprints/Core/PolygonAI/PathNodes/BP_PathNode Object Reference"))
  (locals (`L Nodes` :type "Array of /Game/Blueprints/Core/PolygonAI/PathNodes/BP_PathNode Object Reference"))
  (set `local.L Nodes` `In Nodes`)
  (bind _returnvalue (`KismetArrayLibrary.Array_AddUnique` (`local.L Nodes`) self))
  (if (>= _returnvalue 0)
    (`KismetArrayLibrary.Array_AddUnique` (`local.L Nodes`) self)
    (`|ExecutionSequence`
      (:`then_0`
        (bind _previous_node (`self.Previous Node`)
          (:`then`
            (bind _nodes (`self.Get Previous Node Recursive` _previous_node (`local.L Nodes`)))
            (`KismetArrayLibrary.Array_Append` (`local.L Nodes`) _nodes))
          (:`else`)))
      (:`then_1`
        (return (`local.L Nodes`))))))

(fn `Update Next Node Path Visualiser`
  (bind _next_node (`self.Next Node`)
    (:`then`
      (`SplineComponent.SetLocationAtSplinePoint` (`self.SplineNext`) 1 (+ (`self.K2_GetActorLocation` _next_node) (0.0 0.0 50.0)) "World" true))
    (:`else`
      (`SplineComponent.SetLocationAtSplinePoint` (`self.SplineNext`) 1 (+ (`self.K2_GetActorLocation`) (0.0 0.0 50.0)) "World" true))))

(fn `Update Path Nodes`
  (`|ExecutionSequence`
    (:`then_0`
      (`self.Next Node`
        (:`then`
          (if (== (`self.Next Node`) self)
            (set `self.Next Node` null)
            (else
              (`/Game/Blueprints/Core/PolygonAI/PathNodes/BP_PathNode.Previous Node` (`self.Next Node`)
                (:`then`)
                (:`else`
                  (set `/Game/Blueprints/Core/PolygonAI/PathNodes/BP_PathNode.Previous Node` self (`self.Next Node`)))))))
        (:`else`)))
    (:`then_1`
      (`self.Previous Node`
        (:`then`
          (if (== (`self.Previous Node`) self)
            (set `self.Previous Node` null)
            (else
              (`/Game/Blueprints/Core/PolygonAI/PathNodes/BP_PathNode.Next Node` (`self.Previous Node`)
                (:`then`)
                (:`else`
                  (set `/Game/Blueprints/Core/PolygonAI/PathNodes/BP_PathNode.Next Node` self (`self.Previous Node`)))))))
        (:`else`)))
    (:`then_2`
      (`self.Update Next Node Path Visualiser`)
      (`|ExecutionSequence`
        (:`then_0`
          (bind _next_node (`self.Next Node`)
            (:`then`
              (`self.Update Next Node Path Visualiser` _next_node))
            (:`else`)))
        (:`then_1`
          (bind _previous_node (`self.Previous Node`)
            (:`then`
              (`self.Update Next Node Path Visualiser` _previous_node))
            (:`else`)))))))

(fn `UserConstructionScript`
  (`self.Update Path Nodes`)
  (`TextRenderComponent.K2_SetText` (`self.TextRender`) (`KismetTextLibrary.Conv_StringToText` (`KismetSystemLibrary.GetDisplayName` self))))