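; BP_StatProgressor is a one-shot actor that increments a named online stat, either per-user or a Steam-aggregated global total shown in the frontend.
; On BeginPlay it checks for an online subsystem, requests stats, then adds IncrementAmount to StatName and stores the result.
; It destroys itself on success or failure.
; The spawner must ensure only the host commits Total_ stats.
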(event `self.ReceiveBeginPlay`
  ;[0.2026 0.5578 1] Note Only host should commit to the Total_ stats (manage this before spawning this, which allows this to progress local user stats OR global stats)
  ; These are aggregated in steam, and shown in the frontend W_GlobalState block
  (if (`/Game/_Guards/OnlineSubsystem/BPFL_OnlineSubsystem.Guards Has Online Subsystem`)
    (`/Game/_Guards/OnlineSubsystem/BPFL_OnlineSubsystem.Request Stats` (delegate `Stats Received`))
    (else
      (`self.K2_DestroyActor`))))

(event `Stats Received`
  (params (Data :type "UserStatsReceived Structure (by ref)"))
  ;[0.2026 0.5578 1] Note Only host should commit to the Total_ stats (manage this before spawning this, which allows this to progress local user stats OR global stats)
  ; These are aggregated in steam, and shown in the frontend W_GlobalState block
  (bind (_data _returnvalue) (`UserStats.GetStatInt` (`self.Stat Name`)))
  (if _returnvalue
    (`UserStats.SetStatInt` (`self.Stat Name`) (+ _data (`self.Increment Amount`)))
    (`UserStats.StoreStats`)
    ;;[1 1 1] Remove after complete
    (`self.K2_DestroyActor`)
    (else
      (`self.K2_DestroyActor`))))

(fn `UserConstructionScript`)