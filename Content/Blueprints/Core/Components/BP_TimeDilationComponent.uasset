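; Actor component that changes global time dilation across a networked game.
; A server event stores the value in a replicated Dilation variable and calls a multicast event, with the OnRep also applying it on clients.
; Both paths run SetDilation, which sets global dilation, fires a change dispatcher and gives the first player controller the inverse custom dilation to offset the effect.
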(event `Server Set Time Dilation`
  (params (`Time Dilation` :type "Float (double-precision)"))
  (bind _output_get (set `self.Dilation` `Time Dilation`))
  (`self.MC Time Dilation` _output_get))

(event `MC Time Dilation`
  (params (InputPin :type "Float (double-precision)"))
  (`self.Set Dilation` InputPin))

(fn `OnRep_Dilation`
  (`self.Set Dilation` (`self.Dilation`)))

(fn `Set Dilation`
  (params (InputPin :type "Float (double-precision)"))
  (bind _returnvalue (`GameplayStatics.GetPlayerController` 0))
  (`GameplayStatics.SetGlobalTimeDilation` InputPin)
  (`self.Time Dilation Changed` InputPin)
  (`/Engine/EditorBlueprintResources/StandardMacros.IsValid` _returnvalue
    (:`Is Valid`
      (set `Actor.CustomTimeDilation` (/ 1.0 InputPin) _returnvalue))))