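; BP_FootstepComponent is an actor component that turns animation motion effects into footstep feedback and noise.
; On a successful hit it executes a local footstep GameplayCue at the trace start to limit audio occlusion, passing the effect tag and physical material.
; On authority, Player-tagged owners also create noise at the impact point, quiet only when sneaking off SurfaceType4.
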(event `GuardsContextEffectInterface.AnimMotionEffect`
  (params (Bone :type Name) (MotionEffect :type "GameplayTag Structure") (StaticMeshComponent :type "SceneComponent Object Reference") (AnimationSequence :type "AnimSequenceBase Object Reference") (bHitSuccess :type Boolean) (HitResult :type "HitResult Structure") (Contexts :type "GameplayTagContainer Structure"))
  (bind (_bblockinghit _binitialoverlap _time _distance _location _impactpoint _normal _impactnormal _physmat _hitactor _hitcomponent _hitbonename _bonename _hititem _elementindex _faceindex _tracestart) (`GameplayStatics.BreakHitResult` HitResult))
  (bind _returnvalue (`self.GetOwner`))
  ;[1 1 1] This component only exists to forward the events. The character can also implement the ContextEffectsInterface.
  (if bHitSuccess
    (`GuardsAbilityFunctionLibrary.ExecuteLocalGameplayCueOnActor` (`self.GetOwner`) (struct :`TagName` "GameplayCue.Movement.Footstep") (`AbilitySystemBlueprintLibrary.MakeGameplayCueParameters` 0.0 0.0 (struct) (struct) MotionEffect (struct) (struct) _tracestart _impactpoint null null null _physmat))
    ;[1 1 1] Noise
    (`/Engine/EditorBlueprintResources/ActorComponentMacros.Switch Has Authority`
      (:`Authority`
        (if (`Actor.ActorHasTag` _returnvalue "Player")
          (`/Game/Blueprints/Core/PolygonAI/SenseData/BPFL_Noise.Create Noise` _returnvalue (+ _impactpoint (0.0 0.0 5.0)) (select `bool` (or (not (== MotionEffect (struct :`TagName` "AnimEffect.Footstep.Sneak"))) (`|EnumEquality` (`PhysicalMaterial.SurfaceType` _physmat) "SurfaceType4")) :`false` (`self.Quiet Step Noise`) :`true` (`self.Loud Step Noise`))))))))