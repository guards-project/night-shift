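; VOIP talker component on a PlayerState that provides attenuated voice chat, attached to the player character's capsule.
; It registers the talker, retries setup on a timer until the pawn is valid, rebinds after pawn destruction, and mute-toggles the talker during setup.
; Mic threshold and gain follow console variables.
; Chat toggles speaking by console command and replicates transmitting state through a server event, while muting applies per talker.
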(event `self.ReceiveBeginPlay`
  (`self.Register Player`)
  (`self.Local Setup`))

(event `Local Setup`
  (`CVarChangeListenerManager.AddFloatCVarCallbackStatic` "Voice.MicThreshold" (delegate `On Mic Threshold Changed`) true)
  (`CVarChangeListenerManager.AddFloatCVarCallbackStatic` "Voice.MicGain" (delegate `On Mic Gain Changed`) true)
  (`KismetSystemLibrary.ExecuteConsoleCommand` "Voice.MicNoiseGateThreshold 0.02" null)
  (`KismetSystemLibrary.ExecuteConsoleCommand` "Voice.SilenceDetectionThreshold 0.02" null))

(event `On Mic Threshold Changed`
  (params (NewValue :type "Float (single-precision)"))
  (`VOIPStatics.SetMicThreshold` NewValue))

(event `On Mic Gain Changed`
  (params (NewValue :type "Float (single-precision)"))
  (`KismetSystemLibrary.ExecuteConsoleCommand` (`KismetStringLibrary.Concat_StrStr` "Voice.MicInputGain " (`KismetStringLibrary.Conv_DoubleToString` NewValue)) null))

(event `On Pawn Destroyed`
  (params (DestroyedActor :type "Actor Object Reference"))
  (`KismetSystemLibrary.Delay` 0.2)
  (`self.Init Voip`))

(event `Set Chatting`
  (params (Chat :type Boolean))
  (`self.Transmitting Changed` Chat)
  (`self.Server Set Transmitting` Chat)
  (if Chat
    (`KismetSystemLibrary.ExecuteConsoleCommand` "ToggleSpeaking 1" null)
    (`KismetSystemLibrary.PrintString` "Talking Started")
    (else
      (`KismetSystemLibrary.ExecuteConsoleCommand` "ToggleSpeaking 0" null)
      (`KismetSystemLibrary.PrintString` "Talking Stopped"))))

(event `Server Set Transmitting`
  (params (Chatting :type Boolean))
  (set `self.Transmitting` Chatting))

(event `self.ReceiveTick`
  (params (DeltaSeconds :type "Float (single-precision)"))
  (bind _asplayer_state (cast `PlayerState` (`self.GetOwner`)))
  (if (!= _asplayer_state (`self.Talker PS`))
    (`self.Register Player`)))

(event `Set Muted`
  (params (Muted :type Boolean))
  (bind _uniquenetid (`AdvancedSessionsLibrary.GetUniqueNetIDFromPlayerState` (`self.Talker PS`)))
  (bind _output_get (set `self.Muted` Muted))
  (`self.Muted Changed` (`self.Muted`))
  (if _output_get
    (`AdvancedVoiceLibrary.MuteRemoteTalker` 0 _uniquenetid)
    (else
      (`AdvancedVoiceLibrary.UnMuteRemoteTalker` 0 _uniquenetid))))

(fn `Init Voip`
  (bind _uniquenetid (`AdvancedSessionsLibrary.GetUniqueNetIDFromPlayerState` (`self.Talker PS`)))
  (bind _talker_ps (`self.Talker PS`)
    (:`then`
      (bind _returnvalue (`PlayerState.GetPawn` _talker_ps))
      (`/Engine/EditorBlueprintResources/StandardMacros.IsValid` _returnvalue
        (:`Is Valid`
          (bind _asbp_character_template_player (cast `/Game/Blueprints/Core/BP_Character_Template_Player` _returnvalue)
            (:`then`
              (set `self.Settings` (make `VoiceSettings` (`Character.CapsuleComponent` _asbp_character_template_player) "/Game/Blueprints/Core/Components/Voice/ATT_VoiceChat.ATT_VoiceChat"))
              (add `Actor.OnDestroyed` _returnvalue (`|CreateDelegate` :!event `On Pawn Destroyed`))
              (`AdvancedVoiceLibrary.MuteRemoteTalker` 0 _uniquenetid)
              (`AdvancedVoiceLibrary.UnMuteRemoteTalker` 0 _uniquenetid))
            (:`CastFailed`
              (`KismetSystemLibrary.K2_SetTimerDelegate` (`|CreateDelegate` :!event `Init Voip`) 0.2 :!label _label))))
        (:`Is Not Valid`
          (goto _label))))
    (:`else`
      (goto _label))))

(fn `OnRep_Transmitting`
  (`self.Transmitting Changed` (`self.Transmitting`)))

(fn `Register Player`
  (bind _asplayer_state (cast `PlayerState` (`self.GetOwner`)))
  (`self.RegisterWithPlayerState` _asplayer_state)
  (set `self.Talker PS` _asplayer_state)
  (`self.Init Voip`))