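; Health component that applies damage and healing to its owner through GAS Companion attributes.
; Caches the GSC core component, retrying until found, and on the server sets default max health and binds point and radial damage to EditHealth.
; EditHealth requires a valid causer and an actual change, blocking damage under Status.Invulnerable.
; It clamps health, broadcasts changed, zero and full events, and reports damage events for AI perception.
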(event `self.ReceiveBeginPlay`
  (`self.Cache GSC Core`)
  (`/Engine/EditorBlueprintResources/ActorComponentMacros.Switch Has Authority`
    (:`Authority`
      (add `Actor.OnTakePointDamage` (`self.GetOwner`) (delegate `On Point Damage`))
      (add `Actor.OnTakeRadialDamage` (`self.GetOwner`) (delegate `On Radial Damage`)))))

(event `Cache GSC Core`
  (bind _returnvalue (`GSCBlueprintFunctionLibrary.GetCompanionCoreComponent` (`self.GetOwner`)))
  (`/Engine/EditorBlueprintResources/StandardMacros.IsValid` _returnvalue
    (:`Is Valid`
      (set `self.GSC Core` _returnvalue)
      (`/Engine/EditorBlueprintResources/ActorComponentMacros.Switch Has Authority`
        (:`Authority`
          (`self.Set Max Health` (`self.Default Health`)))))
    (:`Is Not Valid`
      (`KismetSystemLibrary.PrintString` (`KismetStringLibrary.Concat_StrStr` "Error Cannot find GSC Core Actor: " (`KismetSystemLibrary.GetDisplayName` (`self.GetOwner`))))
      (`KismetSystemLibrary.Delay` 0.2)
      (`self.Cache GSC Core`))))

(event `On Point Damage`
  (params (DamagedActor :type "Actor Object Reference") (Damage :type "Float (single-precision)") (InstigatedBy :type "Controller Object Reference") (HitLocation :type "Vector Structure") (FHitComponent :type "PrimitiveComponent Object Reference") (BoneName :type Name) (ShotFromDirection :type "Vector Structure") (DamageType :type "DamageType Object Reference") (DamageCauser :type "Actor Object Reference"))
  (`self.Edit Health` (* Damage -1.0) DamageType HitLocation (`GameplayStatics.MakeHitResult` true false 0.0 0.0 HitLocation HitLocation ShotFromDirection ShotFromDirection null null null BoneName) InstigatedBy DamageCauser))

(event `On Radial Damage`
  (params (DamagedActor :type "Actor Object Reference") (Damage :type "Float (single-precision)") (DamageType :type "DamageType Object Reference") (Origin :type "Vector Structure") (HitInfo :type "HitResult Structure (by ref)") (InstigatedBy :type "Controller Object Reference") (DamageCauser :type "Actor Object Reference"))
  (`self.Edit Health` (* Damage -1.0) DamageType Origin HitInfo InstigatedBy DamageCauser))

(fn `Can Edit Health`
  (params (Delta :type "Float (double-precision)") (`Damage Type` :type "DamageType Object Reference") (Causer :type "Actor Object Reference"))
  (returns (ReturnValue :type Boolean))
  (locals (`L Parent GAS` :type "AbilitySystemComponent Object Reference"))
  (bind _returnvalue (`self.Get Health`))
  (`/Engine/EditorBlueprintResources/StandardMacros.IsValid` Causer
    (:`Is Valid`
      (if (!= _returnvalue (`KismetMathLibrary.FClamp` (+ _returnvalue (`local.Delta`)) 0.0 (`self.Get Max Health`)))
        ;[1 1 1] Additional Guarding Check if taking damage (not healing)
        (if (< (`local.Delta`) 0.0)
          (return (not (`GSCBlueprintFunctionLibrary.HasMatchingGameplayTag` (`self.GetOwner`) (struct :`TagName` "Status.Invulnerable")))) ; cannot take damage when invulnerable
          (else
            (return true) ; allow healing
          ))
        (else
          (return false) ; return false if health does not change
        )))))

(fn `Edit Health`
  (params (Delta :type "Float (double-precision)") (`Damage Type` :type "DamageType Object Reference") (Origin :type "Vector Structure") (Hit :type "HitResult Structure") (`In Instigator` :type "Controller Object Reference") (Causer :type "Actor Object Reference"))
  (if (`self.Can Edit Health` Delta `Damage Type` Causer)
    (`GSCCoreComponent.SetAttributeValue` (`self.GSC Core`) (struct :`AttributeName` "Health" :`Attribute` "/Script/GASCompanion.GSCAttributeSet:Health" :`AttributeOwner` "/Script/CoreUObject.Class'\"/Script/GASCompanion.GSCAttributeSet\"'") (`KismetMathLibrary.FClamp` (+ (`self.Get Health`) (`local.Delta`)) 0.0 (`self.Get Max Health`)))
    (`self.Health Changed` self (`local.Delta`) (`self.Get Health`) (`local.Damage Type`))
    (`|ExecutionSequence`
      (:`then_0`
        ;[1 1 1] Zero
        (if (== (`self.Get Health`) 0.0)
          (`self.Health Zero` self (`local.In Instigator`) (`local.Causer`) (`local.Hit`) (`local.Damage Type`))))
      (:`then_1`
        ;[1 1 1] Max
        (if (== (`self.Get Health`) (`self.Get Max Health`))
          (`self.Health Full` self)))
      (:`then_2`
        ;[1 1 1] Report Damage
        (if (< (`local.Delta`) 0.0)
          (`AISense_Damage.ReportDamageEvent` (`self.GetOwner`) (`local.In Instigator`) (`local.Delta`) (`local.Origin`) (`.Location` (`GameplayStatics.BreakHitResult` (`local.Hit`))) "Damage"))))))

(fn `Get Health`
  (returns (ReturnValue :type "Float (single-precision)"))
  (return (`.ReturnValue` (`AbilitySystemBlueprintLibrary.GetFloatAttribute` (`self.GetOwner`) (struct :`AttributeName` "Health" :`Attribute` "/Script/GASCompanion.GSCAttributeSet:Health" :`AttributeOwner` "/Script/CoreUObject.Class'\"/Script/GASCompanion.GSCAttributeSet\"'")))))

(fn `Get Max Health`
  (returns (ReturnValue :type "Float (single-precision)"))
  (return (`.ReturnValue` (`AbilitySystemBlueprintLibrary.GetFloatAttribute` (`self.GetOwner`) (struct :`AttributeName` "MaxHealth" :`Attribute` "/Script/GASCompanion.GSCAttributeSet:MaxHealth" :`AttributeOwner` "/Script/CoreUObject.Class'\"/Script/GASCompanion.GSCAttributeSet\"'")))))

(fn `Reset Health`
  (`self.Set Health` (`self.Get Max Health`)))

(fn `Set Default Health`
  (params (`Default Health` :type "Float (double-precision)"))
  (set `self.Default Health` `Default Health`)
  (`self.Set Max Health` (`self.Default Health`))
  (`self.Set Health` (`self.Default Health`)))

(fn `Set Health`
  (params (NewValue :type "Float (single-precision)"))
  (bind _gsc_core (`self.GSC Core`)
    (:`then`
      (`GSCCoreComponent.SetAttributeValue` _gsc_core (struct :`AttributeName` "Health" :`Attribute` "/Script/GASCompanion.GSCAttributeSet:Health" :`AttributeOwner` "/Script/CoreUObject.Class'\"/Script/GASCompanion.GSCAttributeSet\"'") NewValue))
    (:`else`)))

(fn `Set Max Health`
  (params (NewValue :type "Float (single-precision)"))
  (bind _gsc_core (`self.GSC Core`)
    (:`then`
      (`GSCCoreComponent.SetAttributeValue` _gsc_core (struct :`AttributeName` "MaxHealth" :`Attribute` "/Script/GASCompanion.GSCAttributeSet:MaxHealth" :`AttributeOwner` "/Script/CoreUObject.Class'\"/Script/GASCompanion.GSCAttributeSet\"'") NewValue))
    (:`else`)))