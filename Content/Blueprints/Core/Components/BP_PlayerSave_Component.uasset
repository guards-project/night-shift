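; Player save component, apparently on the PlayerState, that manages a local player's saved wins and latest mission.
; On BeginPlay, only for the local PlayerController, it loads the "Player" save slot, replacing an invalid save with a fresh SaveGame_Player object.
; AddWin and SetLatestMission delegate to the save object, while ServerSetWins mirrors the win count onto the component after loading an existing save or adding a win.
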(event `self.ReceiveBeginPlay`
  (bind _returnvalue (`self.GetOwner`))
  (bind _returnvalue_2 (`Actor.GetOwner` _returnvalue))
  (`/Engine/EditorBlueprintResources/StandardMacros.IsValid` _returnvalue
    (:`Is Valid`
      (`/Engine/EditorBlueprintResources/StandardMacros.IsValid` _returnvalue_2
        (:`Is Valid`
          (bind _asplayer_controller (cast `PlayerController` _returnvalue_2))
          (if (`Controller.IsLocalPlayerController` _asplayer_controller)
            (`self.Init Save`)))))))

(event `Server Set Wins`
  (params (Wins :type Integer))
  (set `self.Wins` Wins))

(fn `Add Win`
  (bind _save (`self.Save`)
    (:`then`
      (`/Game/Blueprints/Core/PlayerSave/SaveGame_Player.Add Win` _save)
      (`self.Server Set Wins` (`/Game/Blueprints/Core/PlayerSave/SaveGame_Player.Wins` _save)))
    (:`else`)))

(fn `Init Save`
  (bind _returnvalue (`GameplayStatics.DoesSaveGameExist` "Player"))
  (if _returnvalue
    (bind _returnvalue_2 (`GameplayStatics.LoadGameFromSlot` "Player"))
    (`/Engine/EditorBlueprintResources/StandardMacros.IsValid` _returnvalue_2
      (:`Is Valid`
        (bind _assave_game_player (cast `/Game/Blueprints/Core/PlayerSave/SaveGame_Player` _returnvalue_2)
          (:`then`
            (bind _output_get (set `self.Save` _assave_game_player))
            (`self.Server Set Wins` (`/Game/Blueprints/Core/PlayerSave/SaveGame_Player.Wins` _output_get)))
          (:`CastFailed`
            (`GameplayStatics.DeleteGameInSlot` "Player" :!label _label)
            (bind _returnvalue_3 (`GameplayStatics.CreateSaveGameObject` "/Game/Blueprints/Core/PlayerSave/SaveGame_Player.SaveGame_Player_C" :!label _label_2))
            (set `self.Save` _returnvalue_3))))
      (:`Is Not Valid`
        (goto _label)))
    (else
      (goto _label_2))))

(fn `Set Latest Mission`
  (params (`Latest Mission` :type Integer))
  (bind _save (`self.Save`)
    (:`then`
      (`/Game/Blueprints/Core/PlayerSave/SaveGame_Player.Set Latest Mission` _save `Latest Mission`))
    (:`else`)))