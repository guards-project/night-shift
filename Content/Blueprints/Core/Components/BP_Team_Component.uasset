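; Actor component that holds team affiliation and decides whether one team component may target another.
; The Team RepNotify fires the TeamChanged dispatcher with the new team.
; CanTarget requires a targetable other component on a different, non-allied team, plus this component's CanTargetEnemies flag.
; SameTeam simply negates CanTarget for valid components, so untargetable ones also count as same team.
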(fn `Can Target`
  (params (`Other Team` :type "/Game/Blueprints/Core/Components/BP_Team_Component Object Reference"))
  (returns (ReturnValue :type Boolean))
  (locals (NewLocalVar_0 :type "/Game/Blueprints/Core/Components/BP_Team_Component Object Reference"))
  (bind _team (`/Game/Blueprints/Core/Components/BP_Team_Component.Team` (`local.Other Team`)))
  (if (`/Game/Blueprints/Core/Components/BP_Team_Component.Can Be Targetted` (`local.Other Team`))
    (return (and (and (!= _team (`self.Team`)) (not (`KismetArrayLibrary.Array_Contains` (`self.Allied Teams`) _team))) (`self.Can Target Enemies`)))
    (else
      (return false))))

(fn `OnRep_Team`
  (`self.Team Changed` (`self.Team`)))

(fn `Same Team`
  (params (`Other Team Comp` :type "Self Object Reference"))
  (returns (ReturnValue :type Boolean))
  (`/Engine/EditorBlueprintResources/StandardMacros.IsValid` `Other Team Comp`
    (:`Is Valid`
      (return (not (`self.Can Target` self `Other Team Comp`))))
    (:`Is Not Valid`
      (return false))))