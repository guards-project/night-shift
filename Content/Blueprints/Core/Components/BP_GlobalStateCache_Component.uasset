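; Component that pushes stored player stats to the online subsystem and records patrol, district and hostage totals.
; On BeginPlay it calls StoreStats if the subsystem guard passes; a true result prints a failure message, while false retries after a one-second delay.
; Increment events spawn a BP_StatProgressor actor with the stat name chosen by win or loss, or with a count for hostages.
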(event `self.ReceiveBeginPlay`
  (`self.Try Send Stats`))

(event `Try Send Stats`
  (if (`/Game/_Guards/OnlineSubsystem/BPFL_OnlineSubsystem.Guards Has Online Subsystem`)
    (bind _returnvalue (`UserStats.StoreStats`))
    (if _returnvalue
      (`KismetSystemLibrary.PrintString` "Failed to send stats")
      (else
        (`KismetSystemLibrary.Delay` 1.0)
        (`self.Try Send Stats`)))))

(event `Increment Patrols`
  (params (Win :type Boolean))
  (`|SpawnActorFromClass` "/Game/Blueprints/Core/Components/BP_StatProgressor.BP_StatProgressor_C" (`KismetMathLibrary.Conv_VectorToTransform` (0.0 0.0 0.0)) "AlwaysSpawn" "MultiplyWithRoot" null (select `bool` Win :`false` "Total_PatrolsLost" :`true` "Total_PatrolsWon") 1 null))

(event `Increment Kingpin`
  (params (Win :type Boolean))
  (`|SpawnActorFromClass` "/Game/Blueprints/Core/Components/BP_StatProgressor.BP_StatProgressor_C" (`KismetMathLibrary.Conv_VectorToTransform` (0.0 0.0 0.0)) "AlwaysSpawn" "MultiplyWithRoot" null (select `bool` Win :`false` "Total_DistrictFails" :`true` "Total_DistrictWins") 1 null))

(event `Increment Hostages`
  (params (Count :type Integer))
  (`|SpawnActorFromClass` "/Game/Blueprints/Core/Components/BP_StatProgressor.BP_StatProgressor_C" (`KismetMathLibrary.Conv_VectorToTransform` (0.0 0.0 0.0)) "AlwaysSpawn" "MultiplyWithRoot" null "Total_Hostages" Count null))