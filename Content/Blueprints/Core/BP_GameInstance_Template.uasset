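; Game instance that sets up player settings, manages online session joins and exits, and records the last network, travel or kick error.
; Init registers console-variable settings with callbacks for language, scalability, subtitles and colorblind mode, enables VSync and deletes crisis saves.
; Network or travel failures and shutdown delete those saves, destroy the session and send the game state to EntryMap.
; Accepted invites retry until a player controller exists, then leave the current session, join and show a loading screen.
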(event `self.HandleNetworkError`
  (params (FailureType :type "ENetworkFailure Enum" :default "NetDriverAlreadyExists") (bIsServer :type Boolean))
  (`self.Set Error` true FailureType)
  (`self.End Session` :!label _label))

(event `End Session`
  (`/Engine/EditorBlueprintResources/StandardMacros.IsValid` (`GameplayStatics.GetPlayerController` 0)
    (:`Is Valid`
      (`self.Delete Crisis Save Data`)
      (`DestroySessionCallbackProxy.DestroySession` (`GameplayStatics.GetPlayerController` 0)
        (:`OnSuccess`
          _)
        (:`OnFailure`
          _))
      (bind _returnvalue (`GameplayStatics.GetCurrentLevelName` true))
      (if (`KismetStringLibrary.NotEqual_StrStr` _returnvalue "EntryMap")
        (bind _asbp_game_state_guards (cast `/Game/Blueprints/Core/BP_GameState_Guards` (`GameplayStatics.GetGameState`)))
        (`/Game/Blueprints/Core/BP_GameState_Guards.Go to Level` _asbp_game_state_guards "EntryMap")))))

(event `self.HandleTravelError`
  (params (FailureType :type "ETravelFailure Enum" :default "NoLevel"))
  (`self.Set Error` false "NetDriverAlreadyExists" FailureType)
  (goto _label))

(event `self.ReceiveShutdown`
  (`self.End Session`))

(event `self.ReceiveInit`
  ;[1 1 1] Enable VSync
  (`parent.ReceiveInit`)
  (`self.Init CVARs`)
  (`self.Delete Crisis Save Data`)
  (bind _returnvalue (`GameUserSettings.GetGameUserSettings`))
  (`/Engine/EditorBlueprintResources/StandardMacros.IsValid` _returnvalue
    (:`Is Valid`
      (`GameUserSettings.SetVSyncEnabled` _returnvalue true)
      (`GameUserSettings.ApplySettings` _returnvalue true))))

(event `Init CVARs`
  ;[1 1 1] CVAR Settings
  (`SettingsManager.RegisterFloatCVarSetting` "r.TonemapperGamma" 2.0)
  (`SettingsManager.RegisterFloatCVarSetting` "Camera.FOV" 110.0)
  (`SettingsManager.RegisterFloatCVarSetting` "r.ScreenPercentage" 50.0)
  ;;[1 1 1] Mouse / controller sensitivity
  (`SettingsManager.RegisterFloatCVarSetting` "Input.Sensitivity" 1.0)
  (`SettingsManager.RegisterFloatCVarSetting` "Input.PadSensitivity" 1.3)
  (`SettingsManager.RegisterBoolCVarSetting` "Input.HoldSprint" true)
  (`SettingsManager.RegisterBoolCVarSetting` "Input.InvertX")
  (`SettingsManager.RegisterBoolCVarSetting` "Input.InvertY")
  (`SettingsManager.RegisterIntCVarSettingWithCallback` "Game.Lang" (`KismetArrayLibrary.Array_Find` (`KismetInternationalizationLibrary.GetLocalizedCultures` true) (`KismetInternationalizationLibrary.GetCurrentCulture`)) "" (delegate `Lang Changed`) true)
  (`SettingsManager.RegisterBoolCVarSetting` "Host.Private" true)
  (`SettingsManager.RegisterIntCVarSetting` "Host.PlayerCount" 4)
  ;[1 1 1] Game
  (`SettingsManager.RegisterBoolCVarSetting` "Game.Blood" true)
  (`SettingsManager.RegisterIntCVarSetting` "Game.MinBalance" 1)
  (`SettingsManager.RegisterBoolCVarSetting` "Game.IgnoreSoloWarning")
  (`SettingsManager.RegisterBoolCVarSetting` "Host.Locked")
  (`SettingsManager.RegisterBoolCVarSetting` "r.DynamicGlobalIlluminationMethod" true)
  (`SettingsManager.RegisterFloatCVarSetting` "Voice.MicThreshold" -1.0)
  (`SettingsManager.RegisterFloatCVarSetting` "Voice.MicGain" 2.5)
  (`SettingsManager.RegisterIntCVarSettingWithCallback` "video.scalability" 2 "" (delegate `Scalability Changed`) true)
  (`SettingsManager.RegisterBoolCVarSettingWithCallback` "Game.Subtitles" false "" (delegate `Subtitles Changed`) true)
  (`SettingsManager.RegisterBoolCVarSetting` "Game.DisableHeadBob")
  (`SettingsManager.RegisterIntCVarSettingWithCallback` "Color.Mode" 0 "" (delegate `Color Mode Changed`))
  (`SettingsManager.RegisterFloatCVarSettingWithCallback` "Color.Severity" 1.0 "" (delegate `Color Severity Changed`) true)
  (`SettingsManager.RegisterIntCVarSetting` "Balance.EnemyFreq" 1)
  (`SettingsManager.RegisterBoolCVarSetting` "Balance.FF" true))

(event `Color Mode Changed`
  (params (NewValue :type Integer))
  (`WidgetBlueprintLibrary.SetColorVisionDeficiencyType` (cast `EColorVisionDeficiency` (`KismetMathLibrary.Conv_IntToByte` (`ConsoleUtils.GetIntCVar` "Color.Mode"))) (`ConsoleUtils.GetFloatCVar` "Color.Severity") true :!label _label_2))

(event `Color Severity Changed`
  (params (NewValue :type "Float (single-precision)"))
  (goto _label_2))

(event `Scalability Changed`
  (params (NewValue :type Integer))
  (bind _returnvalue (`GameUserSettings.GetGameUserSettings`))
  (`GameUserSettings.SetOverallScalabilityLevel` _returnvalue NewValue)
  (`GameUserSettings.ApplySettings` _returnvalue true))

(event `Subtitles Changed`
  (params (NewValue :type Boolean))
  (`GameplayStatics.SetSubtitlesEnabled` NewValue))

(event `Lang Changed`
  (params (NewValue :type Integer))
  (`KismetInternationalizationLibrary.SetCurrentCulture` (`|GetArrayItem` (`KismetInternationalizationLibrary.GetLocalizedCultures` true) NewValue)))

(event `self.OnSessionInviteAccepted`
  (params (LocalPlayerNum :type Integer) (PersonInvited :type "BPUniqueNetId Structure") (SessionToJoin :type "BlueprintSessionResult Structure (by ref)"))
  ;[1 1 1] Join Session
  (set `self.Session To Join` SessionToJoin)
  (`self.Join Accepted Session`))

(event `Join Accepted Session`
  ;[1 1 1] Join Session
  (`/Engine/EditorBlueprintResources/StandardMacros.IsValid` (`GameplayStatics.GetPlayerController` 0)
    (:`Is Valid`
      (`self.Join Guards Session` (`self.Session To Join`)))
    (:`Is Not Valid`
      (`KismetSystemLibrary.K2_SetTimerDelegate` (delegate `Join Accepted Session`) 1.0))))

(event `Join Guards Session`
  (params (SearchResult :type "BlueprintSessionResult Structure (by ref)"))
  (bind _returnvalue (`GameplayStatics.GetPlayerController` 0))
  ;[1 1 1] Join Session
  (`DestroySessionCallbackProxy.DestroySession` _returnvalue
    (:`OnSuccess`
      _)
    (:`OnFailure`
      _))
  (`JoinSessionCallbackProxy.JoinSession` _returnvalue SearchResult
    (:`OnSuccess`
      (`WidgetLayoutLibrary.RemoveAllWidgets`)
      (bind _returnvalue_2 (`|CreateWidget` "/Game/_Guards/UserInterface/LoadingScreen/W_LoadingScreen_Default.W_LoadingScreen_Default_C" (`GameplayStatics.GetPlayerController` 0)))
      (`UserWidget.AddToViewport` _returnvalue_2 1))))

(fn `Delete Crisis Save Data`
  (for _array_element (`self.DeleteSaves`)
    (bind _returnvalue (`GameplayStatics.DoesSaveGameExist` _array_element))
    (if _returnvalue
      (`GameplayStatics.DeleteGameInSlot` _array_element))))

(fn `Set Error`
  (params (`Is Network Failure` :type Boolean) (`Network Type` :type "ENetworkFailure Enum" :default "NetDriverAlreadyExists") (`Travel Type` :type "ETravelFailure Enum" :default "NoLevel"))
  (set `self.Last Error` (make `/Game/Blueprints/Core/Components/ErrorHandler/F_Error` (select `bool` `Is Network Failure` :`false` "Travel Error" :`true` "Network Error" :!type "Text") (select `bool` (`|EnumEquality` `Network Type` "ConnectionLost") :`false` (`KismetTextLibrary.Conv_StringToText` (`KismetMathLibrary.SelectString` (`|GetEnumeratorNameAsString` `Network Type`) (`|GetEnumeratorNameAsString` `Travel Type`) `Is Network Failure`)) :`true` "SessionEnded"))))

(fn `Set Kick Reason`
  (params (Title :type Text) (Text :type Text))
  (set `self.Last Error` (make `/Game/Blueprints/Core/Components/ErrorHandler/F_Error` Title Text)))