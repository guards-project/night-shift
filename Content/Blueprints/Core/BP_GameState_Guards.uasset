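; Game state for the Guards multiplayer game, running the mission round, map travel and lobby hosting.
; The server tracks round time and ends the round when no player is left alive, disabling AI senses, awarding win coins and returning to the HUB on a timer.
; HUB and training deaths enter a revive queue instead.
; Travel saves inventory, shows per-mission loading screens, then uses ServerTravel or OpenLevel; hosting creates an advanced session.
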(event `self.ReceiveBeginPlay`
  ;[1 1 1] Round Time set by server - offset by time since this GameState instance was made (after map travel)
  ; because server world time returns full time since server was up
  (`/Engine/EditorBlueprintResources/ActorMacros.Switch Has Authority`
    (:`Authority`
      (set `self.Start Stamp` (`self.GetServerWorldTimeSeconds`))
      (`self.Reset`))))

(event `self.ReceiveTick`
  (params (DeltaSeconds :type "Float (single-precision)"))
  ;[1 1 1] Round Time set by server - offset by time since this GameState instance was made (after map travel)
  ; because server world time returns full time since server was up
  (`/Engine/EditorBlueprintResources/ActorMacros.Switch Has Authority`
    (:`Authority`
      (set `self.Round Time` (- (`self.GetServerWorldTimeSeconds`) (`self.Start Stamp`))))))

(event `MC End Round`
  (params (Win :type Boolean) (Context :type "Transform Structure") (Timeout :type Boolean))
  ;[1 1 1] End Round
  (`/Engine/EditorBlueprintResources/StandardMacros.DoOnce` false :!label _label
    (:`Completed`
      (set `self.Win` Win)
      (set `self.Timeout` Timeout)
      (`self.Update End Of Round Time`)
      (`self.Cleanup Gameplay`)
      (bind _returnvalue (`KismetSystemLibrary.K2_SetTimerDelegate` (delegate `Go To HUB`) (`self.End Round Duration`)))
      (set `self.End Timer` _returnvalue)
      (`self.Give Coins`)
      (`/Engine/EditorBlueprintResources/StandardMacros.Can Execute Cosmetic Events`
        (:`True`
          (`/Engine/EditorBlueprintResources/StandardMacros.IsValid` (`Controller.K2_GetPawn` (`GameplayStatics.GetPlayerController` 0))
            (:`Is Valid`
              (`self.Update Latest Mission`)
              (`/Game/_Guards/UserInterface/Menus/Stack/BPFL_CommonStack.Push Menu` "/Game/_Guards/UserInterface/AAR/W_AfterActionReport.W_AfterActionReport_C")
              (`self.End Cam` Context))))))))

(event `Reset`
  ;[1 1 1] End Round
  (goto _label :!via `Reset`))

(event `Go To HUB`
  ;[1 1 1] End Round
  (`/Engine/EditorBlueprintResources/ActorMacros.Switch Has Authority`
    (:`Authority`
      (`/Game/Blueprints/Core/Score/BP_Score_Component.Reset` (`self.BP_Score_Component`))
      (`self.Go to Level` (`/Game/Blueprints/Core/BPFL_Guards.Get HUB World`)))))

(event `Revive Next`
  ;[1 1 1] Revive Queue
  (`KismetSystemLibrary.Delay` 2.0)
  (if (`KismetArrayLibrary.Array_IsValidIndex` (`self.Revive Queue`))
    (message `/Game/Blueprints/Core/BPI_Character.Revive` (`|GetArrayItem` (`self.Revive Queue`)))
    (`KismetArrayLibrary.Array_Remove` (`self.Revive Queue`))
    (`self.Revive Next`)))

(event `Cleanup Gameplay`
  ;[1 1 1 1 20] FIXED
  ; AWESOME!
  (`/Engine/EditorBlueprintResources/ActorMacros.Switch Has Authority`
    (:`Authority`
      (bind _outactors (`GameplayStatics.GetAllActorsOfClass` "/Game/Blueprints/Core/PolygonAI/BP_Polygon_AI.BP_Polygon_AI_C"))
      (for _array_element _outactors
        (bind _returnvalue (`AIBlueprintHelperLibrary.GetAIController` _array_element))
        (`/Engine/EditorBlueprintResources/StandardMacros.IsValid` _returnvalue
          (:`Is Valid`
            (bind _asai_controller_polygon (cast `/Game/Blueprints/Core/PolygonAI/Behaviour/AI_Controller_Polygon` _returnvalue))
            (`/Game/Blueprints/Core/PolygonAI/Behaviour/AI_Controller_Polygon.Set AI Senses Enabled` _asai_controller_polygon false)))))))

(event `Write Achievement for level`
  (params (AchievementName :type Name))
  ;[1 1 1] Achievement per Mission
  (`AchievementQueryCallbackProxy.CacheAchievements` (`GameplayStatics.GetPlayerController` 0)
    (:`OnSuccess`
      (`AchievementWriteCallbackProxy.WriteAchievementProgress` (`GameplayStatics.GetPlayerController` 0) AchievementName))))

(event `Go to Level`
  (params (LevelName :type Name))
  ;[1 1 1] Travel Between Maps
  (set `self.Guards Travelling` true)
  (`self.Cache Player Count`)
  (`self.MC Loading Screen` (`KismetStringLibrary.Conv_NameToString` LevelName))
  (`KismetSystemLibrary.Delay` 3.0)
  (`|ExecutionSequence`
    (:`then_0`
      (`/Engine/EditorBlueprintResources/ActorMacros.Switch Has Authority` ; if server, cleanup session
        (:`Authority`
          (`/Game/Primer/Primer_MissionHierarchy/BP_MissionRegistry_Component.Destroy All Missions` (`self.BP_MissionRegistry_Component_Guards`)))))
    (:`then_1`
      (if (or (`KismetSystemLibrary.IsStandalone`) (not (`KismetSystemLibrary.IsServer`)))
        (`GameplayStatics.OpenLevel` LevelName)
        (else
          (`AdvancedSessionsLibrary.ServerTravel` (`KismetStringLibrary.Conv_NameToString` LevelName)))))))

(event `MC Loading Screen`
  (params (MapName :type String))
  ;[1 1 1] Travel Between Maps
  (`self.Local Player Save Persistent Inventory`)
  (`self.Disable Physical Animation`)
  (`PlayerCameraManager.StartCameraFade` :`self` (`GameplayStatics.GetPlayerCameraManager` 0) :`ToAlpha` 1.0 :`Duration` 0.5 :`bHoldWhenFinished` true)
  (`KismetSystemLibrary.Delay` 0.6)
  (bind _returnvalue (`|CreateWidget` (`self.Get Loading Screen Class` MapName)))
  (`UserWidget.AddToViewport` _returnvalue 0)
  (`/Game/Blueprints/Core/BPFL_Guards.Remove All Widgets Except` (`|MakeArray` _returnvalue)))

(event `Disable Physical Animation`
  ;[1 1 1] Crash Fix (get all character templates and disable physical animation
  (bind _outactors (`GameplayStatics.GetAllActorsOfClass` "/Script/Engine.Character"))
  (for _array_element _outactors
    (`/Engine/EditorBlueprintResources/StandardMacros.IsValid` _array_element
      (:`Is Valid`
        (message `/Game/Blueprints/Core/BPI_Character.Disable Physical Animation` _array_element)))))

(event `Start Host Lobby`
  ;[1 1 1] Create Session
  (bind _asbp_game_instance_template (cast `/Game/Blueprints/Core/BP_GameInstance_Template` (`GameplayStatics.GetGameInstance`)))
  (`/Game/Blueprints/Core/BP_GameInstance_Template.Delete Crisis Save Data` _asbp_game_instance_template)
  (bind _returnvalue (`Utils.GetIPCountry`))
  (`CreateSessionCallbackProxyAdvanced.CreateAdvancedSession` (`|MakeArray` (`AdvancedSessionsLibrary.MakeLiteralSessionPropertyString` "Game" "Guards") (`AdvancedSessionsLibrary.MakeLiteralSessionPropertyString` "ServerName" (`KismetStringLibrary.Concat_StrStr` (`PlayerState.GetPlayerName` (`Controller.PlayerState` (`GameplayStatics.GetPlayerController` 0))) "'s Server")) (`AdvancedSessionsLibrary.MakeLiteralSessionPropertyBool` "Locked" (`ConsoleUtils.GetBoolCVar` "Host.Locked")) (`AdvancedSessionsLibrary.MakeLiteralSessionPropertyString` "BuildVersion" (`KismetTextLibrary.Conv_TextToString` (`/Game/Blueprints/Core/BPFL_Guards.Get Build ID`))) (`AdvancedSessionsLibrary.MakeLiteralSessionPropertyString` "Country" _returnvalue) (`AdvancedSessionsLibrary.MakeLiteralSessionPropertyBool` "FF" (`ConsoleUtils.GetBoolCVar` "Balance.FF")) (`AdvancedSessionsLibrary.MakeLiteralSessionPropertyInt` "Difficulty" (`ConsoleUtils.GetIntCVar` "Balance.EnemyFreq"))) (`GameplayStatics.GetPlayerController` 0) (`ConsoleUtils.GetIntCVar` "Host.PlayerCount")
    (:`OnSuccess`
      (`self.MC Loading Screen` (`KismetStringLibrary.Conv_NameToString` (`/Game/Blueprints/Core/BPFL_Guards.Get HUB World`)))
      (`KismetSystemLibrary.Delay` 2.0)
      (`GameplayStatics.OpenLevel` (`/Game/Blueprints/Core/BPFL_Guards.Get HUB World`) true "?listen"))))

(event `self.BP_PlayerJoinLeaveCallback.Player Left`
  (params (Controller :type "Controller Object Reference") (PlayerState :type "PlayerState Object Reference"))
  ;[1 1 1] Check mission loss if a player leaves while remainders are dead
  (`self.Check Loss`))

(fn `Cache Player Count`
  (locals (`L Save` :type "/Game/Blueprints/Crisis/BP_SaveGame_Crisis Object Reference"))
  (bind _l_save (`local.L Save`))
  (`/Engine/EditorBlueprintResources/ActorMacros.Switch Has Authority`
    (:`Authority`
      (bind _returnvalue (`/Game/Blueprints/Crisis/BPFL_Crisis.Get Crisis Component` ""))
      (bind _crisis_save (`/Game/Blueprints/Crisis/BP_Crisis_Component.Get Crisis Save` _returnvalue))
      (set `local.L Save` _crisis_save)
      (set `/Game/Blueprints/Crisis/BP_SaveGame_Crisis.Player Count` (`KismetArrayLibrary.Array_Length` (`self.PlayerArray`)) _l_save)
      (`/Game/Blueprints/Crisis/BP_SaveGame_Crisis.Save` _l_save))))

(fn `Check Loss`
  (locals (`L Found Living Player` :type Boolean :default false) (`L Context` :type "Transform Structure") (`L Living Guards` :type "Array of /Game/Blueprints/Core/BP_Character_Template_Player Object Reference"))
  (`/Engine/EditorBlueprintResources/ActorMacros.Switch Has Authority`
    (:`Authority`
      (bind _outactors (`GameplayStatics.GetAllActorsOfClass` "/Game/Blueprints/Core/BP_Character_Template_Player.BP_Character_Template_Player_C"))
      (for _array_element _outactors
        (`/Engine/EditorBlueprintResources/StandardMacros.IsValid` _array_element
          (:`Is Valid`
            (bind _dead (message `/Game/Blueprints/Core/BPI_Character.Is Dead` _array_element))
            (bind _ko (message `/Game/Blueprints/Core/BPI_Character.Is KO` _array_element))
            (if (or _ko _dead)
              (bind _returnvalue (`KismetArrayLibrary.Array_AddUnique` (`self.Recently Deceased`) _array_element))
              (if (>= _returnvalue 0)
                (set `local.L Context` (`self.GetTransform` _array_element)))
              (else
                (set `local.L Found Living Player` true)
                (`KismetArrayLibrary.Array_RemoveItem` (`self.Recently Deceased`) _array_element)
                (`KismetArrayLibrary.Array_AddUnique` (`local.L Living Guards`) _array_element))))))
      (if (not (`local.L Found Living Player`))
        (`self.MC End Round` false (`local.L Context`))
        (elif (and (== (`KismetArrayLibrary.Array_Length` (`local.L Living Guards`)) 1) (!= (`KismetArrayLibrary.Array_Length` _outactors) 1))
          (`/Game/Blueprints/Core/BP_Character_Template_Player.Last Guard Standing` (`|GetArrayItem` (`local.L Living Guards`))))))))

(fn `End Cam`
  (params (SpawnTransform :type "Transform Structure"))
  (`|SpawnActorFromClass` "/Game/Blueprints/Gameflow/EndCam/BP_EndCam.BP_EndCam_C" SpawnTransform "AlwaysSpawn" "MultiplyWithRoot" null null))

(fn `Get Loading Screen Class`
  (params (InputPin :type String))
  (returns (`Loading Screen` :type "UserWidget Class Reference"))
  (bind _outrownames (`DataTableFunctionLibrary.GetDataTableRowNames` "/Game/_Guards/UserInterface/WorldMap/DT_Missions.DT_Missions"))
  (for _array_element _outrownames
    (bind _returnvalue (`|GetDataTableRow` "/Game/_Guards/UserInterface/WorldMap/DT_Missions.DT_Missions" _array_element)
      (:`then`
        (bind ((`LevelName_3_A4AFF82645491289FF83C88B1F78F9FF` _levelname) (`LoadingScreen_24_6FE6A7E84912CC1DC37D5A960D53FB30` _loadingscreen)) (break `/Game/_Guards/UserInterface/WorldMap/F_World` _returnvalue))
        (if (`KismetStringLibrary.EqualEqual_StrStr` (`KismetStringLibrary.ToLower` _levelname) (`KismetStringLibrary.ToLower` (`KismetStringLibrary.RightChop` InputPin (+ (`KismetStringLibrary.FindSubstring` InputPin "/" false true) 1))))
          (return _loadingscreen)))))
  (return "/Game/_Guards/UserInterface/LoadingScreen/W_LoadingScreen_Default.W_LoadingScreen_Default_C"))

(fn `Get Mission Time`
  (returns (ReturnValue :type "Float (double-precision)"))
  (return (`self.Round Time`)))

(fn `Give Coins`
  (if (`self.Win`)
    (`/Engine/EditorBlueprintResources/ActorMacros.Switch Has Authority`
      (:`Authority`
        (bind (_array_index _row _data) (`/Game/Blueprints/Core/BPFL_Guards.Get Level Info`))
        (for _array_element (`GameStateBase.PlayerArray` (`GameplayStatics.GetGameState`))
          (bind ((`Coins_44_F0F1B7D840D2D17D6001FBB998AF498A` _coins)) (break `/Game/_Guards/UserInterface/WorldMap/F_World` _data))
          (`/Game/Blueprints/Core/Score/BPFL_Score.Add Score` (`PlayerState.GetPlayerName` _array_element) "Coins_Mission" (`KismetMathLibrary.SelectInt` _coins 200 (>= _coins 0))))))))

(fn `Local Player Save Persistent Inventory`
  (bind _returnvalue (`GameplayStatics.GetPlayerPawn` 0))
  (`/Engine/EditorBlueprintResources/StandardMacros.IsValid` _returnvalue
    (:`Is Valid`
      (bind _asbp_character_template (cast `/Game/Blueprints/Core/BP_Character_Template` _returnvalue))
      (`/Game/Blueprints/Items/BP_Inventory_Component.Cache Persistent Inventory` (`/Game/Blueprints/Core/BP_Character_Template.BP_Inventory_Component` _asbp_character_template)))))

(fn `On Player State Changed`
  (params (Character :type "Character Object Reference"))
  (if (or (`/Game/Blueprints/Core/BPFL_Guards.Is HUB`) (`/Game/Blueprints/Core/BPFL_Guards.Is Training`))
    (`KismetArrayLibrary.Array_Add` (`self.Revive Queue`) (`local.Character`))
    (`self.Revive Next`)
    (else
      (`self.Check Loss`))))

(fn `Update End Of Round Time`
  (`/Engine/EditorBlueprintResources/ActorMacros.Switch Has Authority`
    (:`Authority`
      (bind _returnvalue (`self.Get Mission Time`))
      (set `self.End Round Time` _returnvalue))))

(fn `Update Latest Mission`
  (bind _returnvalue (`self.GetComponentByClass` (`Controller.PlayerState` (`GameplayStatics.GetPlayerController` 0)) "/Game/Blueprints/Core/Components/BP_PlayerSave_Component.BP_PlayerSave_Component_C"))
  (`|ExecutionSequence`
    (:`then_0`
      (if (`self.Win`)
        (`/Engine/EditorBlueprintResources/StandardMacros.IsValid` (`GameplayStatics.GetPlayerController` 0)
          (:`Is Valid`
            (bind (_array_index _row _data) (`/Game/Blueprints/Core/BPFL_Guards.Get Level Info`))
            (if (>= _array_index 0)
              (`self.Write Achievement for level` (`KismetStringLibrary.Conv_StringToName` (`.Achievement_65_0DF65C5B4DAC9F0022A4C5A66B4F5B6F` (break `/Game/_Guards/UserInterface/WorldMap/F_World` _data))))
              (bind _returnvalue_2 (+ _array_index 1))
              (`/Game/Blueprints/Core/PlayerSave/SaveGame_Player.Set Latest Mission` (`/Game/Blueprints/Core/Components/BP_PlayerSave_Component.Save` _returnvalue) (`KismetMathLibrary.SelectInt` (`KismetMathLibrary.Min` _returnvalue_2 2) _returnvalue_2 (`/Game/Blueprints/Core/BPFL_Guards.Is Demo`)))
              (`/Game/Blueprints/Core/Components/BP_PlayerSave_Component.Add Win` _returnvalue))))))
    (:`then_1`
      (bind _returnvalue_3 (`/Game/Blueprints/Crisis/BPFL_Crisis.Get Crisis Component` ""))
      (`/Engine/EditorBlueprintResources/StandardMacros.IsValid` _returnvalue_3
        (:`Is Valid`
          (bind _player_save (`/Game/Blueprints/Core/BPFL_Guards.Get Player Save`))
          (`/Game/Blueprints/Core/PlayerSave/SaveGame_Player.Set Highest District` _player_save (`KismetMathLibrary.Conv_ByteToInt` (`/Game/Blueprints/Crisis/BP_Crisis_Component.District ID` _returnvalue_3))))))))

(fn `UserConstructionScript`)