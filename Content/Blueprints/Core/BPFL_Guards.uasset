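; Blueprint function library of game-wide helpers for Guards, covering level identity, build and demo checks, saves, sessions and utilities.
; Level queries match the current map name against DT_CompositeMissions, the hub name or "Training".
; Demo and GM checks depend on packaged builds and the online subsystem, using app ID, achievement and host-lock cvar.
; Other helpers fetch the PlayerState save, join sessions, clear widgets, trace for ground and multicast server-side FX through BP_FXReplicator.
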(fn `Create Networked FX`
  (params (Location :type "Vector Structure") (SystemTemplate :type "NiagaraSystem Object Reference") (Sound :type "SoundBase Object Reference"))
  (bind _returnvalue (`GameplayStatics.GetGameState` null))
  (if (`self.Has Authority` _returnvalue)
    (`/Game/Blueprints/Core/Components/BP_FXReplicator.MC FX` (`Actor.GetComponentByClass` _returnvalue "/Game/Blueprints/Core/Components/BP_FXReplicator.BP_FXReplicator_C") Location SystemTemplate Sound)))

(fn `Generic Join Session`
  (params (WorldContextObject :type "Object Object Reference") (SearchResult :type "BlueprintSessionResult Structure (by ref)"))
  (bind _asbp_game_instance_template (cast `/Game/Blueprints/Core/BP_GameInstance_Template` (`GameplayStatics.GetGameInstance` WorldContextObject)))
  (`/Game/Blueprints/Core/BP_GameInstance_Template.Join Guards Session` _asbp_game_instance_template SearchResult))

(fn `Get Build ID`
  (returns (ID :type Text))
  (bind _asbp_game_instance_template (cast `/Game/Blueprints/Core/BP_GameInstance_Template` (`GameplayStatics.GetGameInstance` null)))
  (return (`KismetTextLibrary.Conv_StringToText` (`/Game/Blueprints/Core/BP_GameInstance_Template.Build` _asbp_game_instance_template))))

(fn `Get HUB World`
  (returns (Name :type Name))
  (return "HubWorld"))

(fn `Get Level Info`
  (returns (`Array Index` :type Integer) (Row :type "DataTableRowHandle Structure") (Data :type "/Game/_Guards/UserInterface/WorldMap/F_World Structure"))
  (bind _outrownames (`DataTableFunctionLibrary.GetDataTableRowNames` "/Game/_Guards/UserInterface/WorldMap/DT_CompositeMissions.DT_CompositeMissions"))
  (for (_array_element _array_index) _outrownames
    (bind _returnvalue (`|GetDataTableRow` "/Game/_Guards/UserInterface/WorldMap/DT_CompositeMissions.DT_CompositeMissions" _array_element)
      (:`then`
        (bind _returnvalue_2 (`GameplayStatics.GetCurrentLevelName` null))
        (if (`KismetStringLibrary.EqualEqual_StrStr` _returnvalue_2 (`.LevelName_3_A4AFF82645491289FF83C88B1F78F9FF` (break `/Game/_Guards/UserInterface/WorldMap/F_World` _returnvalue)))
          (return _array_index (make `DataTableRowHandle` "/Game/_Guards/UserInterface/WorldMap/DT_CompositeMissions.DT_CompositeMissions" _array_element) _returnvalue)))))
  (return -1))

(fn `Get Player Save`
  (returns (`Player Save` :type "/Game/Blueprints/Core/PlayerSave/SaveGame_Player Object Reference"))
  (bind _returnvalue (`GameplayStatics.GetPlayerController` null))
  (`/Engine/EditorBlueprintResources/StandardMacros.IsValid` _returnvalue
    (:`Is Valid`
      (bind _playerstate (`Controller.PlayerState` _returnvalue)
        (:`then`
          (bind _returnvalue_2 (`Actor.GetComponentByClass` _playerstate "/Game/Blueprints/Core/Components/BP_PlayerSave_Component.BP_PlayerSave_Component_C"))
          (`/Engine/EditorBlueprintResources/StandardMacros.IsValid` _returnvalue_2
            (:`Is Valid`
              (return (`/Game/Blueprints/Core/Components/BP_PlayerSave_Component.Save` _returnvalue_2)))
            (:`Is Not Valid`
              _)))
        (:`else`
          _)))
    (:`Is Not Valid`
      _))
  (return null))

(fn `Has Authority`
  (returns (ReturnValue :type Boolean))
  (return (or (`KismetSystemLibrary.IsServer` null) (`KismetSystemLibrary.IsStandalone` null))))

(fn `Is Component On Ground`
  (params (Component :type "SceneComponent Object Reference") (ActorsToIgnore :type "Array of Actor Object Reference (by ref)") (DrawDebugType :type "EDrawDebugTrace Enum" :default "None"))
  (returns (OutHit :type "HitResult Structure") (ReturnValue :type Boolean))
  (locals (`L Start` :type "Vector Structure" :default (0.0 0.0 0.0)))
  (bind _l_start (`local.L Start`))
  (if (`SceneComponent.DoesSocketExist` Component "Pelvis")
    (set `local.L Start` (`SceneComponent.GetSocketLocation` Component "Pelvis"))
    (else
      (set `local.L Start` (`SceneComponent.K2_GetComponentLocation` Component))))
  (bind (_outhit _returnvalue) (`KismetSystemLibrary.LineTraceSingle` (`local.Component`) (+ _l_start (0.0 0.0 10.0)) (+ _l_start (0.0 0.0 -90.0)) "TraceTypeQuery1" false (`local.ActorsToIgnore`) (`local.DrawDebugType`)))
  (return _outhit _returnvalue))

(fn `Is Demo`
  (returns (`Is Demo` :type Boolean))
  (if (`KismetSystemLibrary.IsPackagedForDistribution`)
    (if (`/Game/_Guards/OnlineSubsystem/BPFL_OnlineSubsystem.Guards Has Online Subsystem` null)
      (bind _returnvalue (`Utils.GetAppID`))
      (return (== _returnvalue 2653200))
      (else
        (return true)))
    (else
      (return false))))

(fn `Is End of Demo`
  (returns (`Is End of Demo` :type Boolean))
  (if (`self.Is Demo` null)
    (bind _returnvalue (`/Game/Blueprints/Crisis/BPFL_Crisis.Get Crisis Component` ""))
    (if (`|EnumEquality` (`/Game/Blueprints/Crisis/BP_Crisis_Component.Crisis State` _returnvalue) "NewEnumerator2")
      (return true)
      (else
        (bind _array_index (`self.Get Level Info` null)) ; linear campaign old style
        (return (== _array_index 2))))
    (else
      (return false))))

(fn `Is GM`
  (returns (ReturnValue :type Boolean))
  (if (`KismetSystemLibrary.IsPackagedForDistribution`)
    (if (`/Game/_Guards/OnlineSubsystem/BPFL_OnlineSubsystem.Guards Has Online Subsystem` null)
      (if (and (`self.Has Authority` null) (`ConsoleUtils.GetBoolCVar` "Host.Locked"))
        (bind _bachieved (`UserStats.GetAchievement` "ACH_Law")) ; given in AAR
        (return _bachieved)
        (else
          (return false)))
      (else
        (return false)))
    (else
      (return true))))

(fn `Is HUB`
  (returns (ReturnValue :type Boolean))
  (bind _returnvalue (`GameplayStatics.GetCurrentLevelName` null))
  (return (== _returnvalue (`self.Get HUB World` null))))

(fn `Is Training`
  (returns (ReturnValue :type Boolean))
  (bind _returnvalue (`GameplayStatics.GetCurrentLevelName` null))
  (return (`KismetStringLibrary.Contains` _returnvalue "Training")))

(fn `Remove All Widgets Except`
  (params (`Keep Widgets` :type "Array of UserWidget Object Reference"))
  (bind _foundwidgets (`WidgetBlueprintLibrary.GetAllWidgetsOfClass` null "/Script/UMG.UserWidget"))
  (bind (_arrayindex _arrayelement) (`/Engine/EditorBlueprintResources/StandardMacros.ReverseForEachLoop` _foundwidgets)
    (:`LoopBody`
      (if (not (`KismetArrayLibrary.Array_Contains` `Keep Widgets` _arrayelement))
        (`Widget.RemoveFromParent` _arrayelement)))))

(fn `Save`
  (`GameplayStatics.SaveGameToSlot` null))