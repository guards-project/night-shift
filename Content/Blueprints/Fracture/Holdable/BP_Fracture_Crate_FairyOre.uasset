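; Breakable, holdable fairy ore crate that releases an escaping fairy effect when it explodes.
; MCExplode extends the parent's explosion by starting the escape animation and switching off the crate's point light.
; The escape plays a sound and activates a particle trail, which a half-speed timeline spirals upward from the explosion location by rotating an offset while lerping its height.
; The trail deactivates when the timeline finishes.
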(event `/Game/Blueprints/Fracture/FractureCore/BP_FractureActor.MC Explode`
  (params (Location :type "Vector Structure"))
  (bind _pointlight (`self.PointLight`))
  (`parent.MC Explode` Location)
  (`self.Fairy Escape Animation` Location)
  (`SceneComponent.SetVisibility` _pointlight false false)
  (`ActorComponent.Deactivate` _pointlight))

(event `Fairy Escape Animation`
  (params (Location :type "Vector Structure"))
  (bind _returnvalue (+ (`self.Yaw`) (* (`GameplayStatics.GetWorldDeltaSeconds`) 360.0)))
  (set `self.Last Location` Location)
  (`TimelineComponent.SetPlayRate` (`self.FairyEscapeTImeline`) (/ 1.0 2.0))
  (`SceneComponent.K2_SetWorldLocation` (`self.P_Trail_Fairy`) Location false false)
  (`GameplayStatics.PlaySoundAtLocation` "/Game/_Guards/Audio/Sounds/A_FairyEscape_Cue.A_FairyEscape_Cue" Location (struct) 1.0 1.0 0.0 null null null null)
  (`ActorComponent.Activate` (`self.P_Trail_Fairy`) false)
  (bind (_direction _newtrack_0) (`Timeline|FairyEscapeTImeline` :!via `PlayFromStart`)
    (:`Update`
      (set `self.Yaw` _returnvalue)
      (`SceneComponent.K2_SetWorldLocation` (`self.P_Trail_Fairy`) (+ (`self.Last Location`) (`KismetMathLibrary.GreaterGreater_VectorRotator` (`KismetMathLibrary.MakeVector` 50.0 0.0 (`KismetMathLibrary.Lerp` 50.0 500.0 _newtrack_0)) (`KismetMathLibrary.MakeRotator` 0.0 0.0 _returnvalue))) false false))
    (:`Finished`
      (`ActorComponent.Deactivate` (`self.P_Trail_Fairy`)))))

(fn `UserConstructionScript`
  (`parent.UserConstructionScript`))