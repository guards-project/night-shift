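; Explosive barrel variant of a fracturable holdable prop that shatters and deals area damage when it explodes.
; ServerExplode runs once: it force-breaks the barrel, waits briefly, applies full radial damage and fires a radial impulse over the same radius, then destroys the actor after a delay.
; MCExplode handles the cosmetics, spawning a Niagara effect and sound at the blast location.
; Both events extend the parent class's versions.
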(event `self.ReceiveBeginPlay`
  (`parent.ReceiveBeginPlay`))

(event `self.Server Explode`
  (params (Location :type "Vector Structure"))
  (`parent.Server Explode` Location)
  (`/Engine/EditorBlueprintResources/StandardMacros.DoOnce` false
    (:`Completed`
      (`self.Force Break`)
      (`KismetSystemLibrary.Delay` 0.02)
      (`GameplayStatics.ApplyRadialDamage` :`BaseDamage` (`self.Damage`) :`Origin` Location :`DamageRadius` (`self.Damage Radius`) :`DamageTypeClass` (`self.Damage Type Class_0`) :`DamageCauser` self :`InstigatedByController` (`self.Damage Instigator`) :`bDoFullDamage` true :`DamagePreventionChannel` "ECC_GameTraceChannel6")
      (set `RadialForceComponent.Radius` (`self.Damage Radius`) (`self.RadialForce`))
      (`RadialForceComponent.FireImpulse` (`self.RadialForce`))
      (`KismetSystemLibrary.Delay` 10.0)
      (`self.K2_DestroyActor`))))

(event `self.MC Explode`
  (params (Location :type "Vector Structure"))
  (`parent.MC Explode` Location)
  (`NiagaraFunctionLibrary.SpawnSystemAtLocation` (`self.Niagara`) Location)
  (`GameplayStatics.PlaySoundAtLocation` (`self.Sound_0`) Location (struct) 1.0 1.0 0.0 null null null null))

(fn `UserConstructionScript`
  (`parent.UserConstructionScript`))