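; Flashbang variant of a holdable fracture barrel that breaks, damages, blinds and stuns when it explodes.
; ServerExplode fractures it once, applies full radial damage and a force impulse, then destroys it after a delay.
; MCExplode plays effects, plus a screen fade and tinnitus sound if the local camera faces the blast, with no distance check.
; On authority, it also applies GE_Stun to characters within the damage radius, regardless of facing.
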(event `self.Server Explode`
  (params (Location :type "Vector Structure"))
  (`parent.Server Explode` Location)
  (`/Engine/EditorBlueprintResources/StandardMacros.DoOnce` false
    (:`Completed`
      (`self.Force Break`)
      (`KismetSystemLibrary.Delay` 0.02)
      (`GameplayStatics.ApplyRadialDamage` :`BaseDamage` (`self.Damage`) :`Origin` Location :`DamageRadius` (`self.Damage Radius`) :`DamageTypeClass` (`self.Damage Type Class_0`) :`DamageCauser` self :`InstigatedByController` (`self.Damage Instigator`) :`bDoFullDamage` true :`DamagePreventionChannel` "ECC_GameTraceChannel6")
      (set `RadialForceComponent.Radius` (`self.Damage Radius`) (`self.RadialForce`))
      (`RadialForceComponent.FireImpulse` (`self.RadialForce`))
      (`KismetSystemLibrary.Delay` 10.0)
      (`self.K2_DestroyActor`))))

(event `self.MC Explode`
  (params (Location :type "Vector Structure"))
  (bind _returnvalue (`GameplayStatics.GetPlayerCameraManager` 0))
  (bind _transformcomponent (`PlayerCameraManager.TransformComponent` _returnvalue))
  (`parent.MC Explode` Location)
  (`|ExecutionSequence`
    (:`then_0`
      (`/Engine/EditorBlueprintResources/StandardMacros.Can Execute Cosmetic Events`
        (:`True`
          (`NiagaraFunctionLibrary.SpawnSystemAtLocation` (`self.Niagara`) Location)
          (`GameplayStatics.PlaySoundAtLocation` (`self.Sound_0`) Location (struct) 1.0 1.0 0.0 null null null null)
          (`/Engine/EditorBlueprintResources/StandardMacros.IsValid` _returnvalue
            (:`Is Valid`
              (if (> (`KismetMathLibrary.Dot_VectorVector` (`SceneComponent.GetForwardVector` _transformcomponent) (`KismetMathLibrary.GetDirectionUnitVector` (`SceneComponent.K2_GetComponentLocation` _transformcomponent) Location)) 0.2)
                (`PlayerCameraManager.StartCameraFade` (`GameplayStatics.GetPlayerCameraManager` 0) 0.0 0.95 0.1 (struct :`R` 0.755208 :`G` 0.755208 :`B` 0.755208 :`A` 1.0) false true)
                (bind _returnvalue_2 (`GameplayStatics.CreateSound2D` "/Game/_Guards/Audio/Sounds/Stun/A_TinnitusSimulator_Cue.A_TinnitusSimulator_Cue" 1.0 1.0 0.0 null))
                (bind _output_get (set `self.Flashbang Sound` _returnvalue_2))
                (`AudioComponent.Play` _output_get 0.0)
                (`KismetSystemLibrary.Delay` (`self.Flash duration`))
                (`PlayerCameraManager.StartCameraFade` (`GameplayStatics.GetPlayerCameraManager` 0) 0.95 0.0 3.0 (struct :`R` 0.755208 :`G` 0.755208 :`B` 0.755208 :`A` 1.0) false true)
                (`AudioComponent.FadeOut` (`self.Flashbang Sound`) 3.0 0.0 "Linear")))))))
    (:`then_1`
      (`/Engine/EditorBlueprintResources/ActorMacros.Switch Has Authority`
        (:`Authority`
          (bind _outactors (`KismetSystemLibrary.SphereOverlapActors` Location (`self.Damage Radius`) (`|MakeArray` "ObjectTypeQuery3" :!type "EObjectTypeQuery Enum") "/Game/Blueprints/Core/BP_Character_Template.BP_Character_Template_C"))
          (for _array_element _outactors
            (`AbilitySystemComponent.BP_ApplyGameplayEffectToSelf` :`self` (`AbilitySystemBlueprintLibrary.GetAbilitySystemComponent` _array_element) :`GameplayEffectClass` "/Game/Blueprints/GAS/Effects/GE_Stun.GE_Stun_C")))))))

(fn `UserConstructionScript`
  (`parent.UserConstructionScript`))