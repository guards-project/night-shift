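; AI-only explosive holdable, per its name, that turns its carrier into a walking bomb.
; On equip, the server binds to the owning character's KO, death and gameplay tag events, while cosmetic-capable instances swap the character's mesh to a red material.
; KO or death drops and detonates it after a short delay, while any change to the combo attack tag does so immediately.
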(event `self.On Equipped`
  (params (NewOwner :type "Actor Object Reference"))
  (`parent.On Equipped` NewOwner)
  (bind _asbp_character_template (cast `/Game/Blueprints/Core/BP_Character_Template` NewOwner))
  (`|ExecutionSequence`
    (:`then_0`
      (`/Engine/EditorBlueprintResources/ActorMacros.Switch Has Authority`
        (:`Authority`
          (add `/Game/Blueprints/Core/BP_Character_Template.OnKO` _asbp_character_template (delegate `OnKO_Event`))
          (add `/Game/Blueprints/Core/BP_Character_Template.OnDied` _asbp_character_template (delegate `OnKO_Event`))
          (add `GSCCoreComponent.OnGameplayTagChange` (`/Game/Blueprints/Core/BP_Character_Template.GSCCore` _asbp_character_template) (delegate `OnGameplayTagChange_Event`)))))
    (:`then_1`
      (`/Engine/EditorBlueprintResources/StandardMacros.Can Execute Cosmetic Events`
        (:`True`
          (`PrimitiveComponent.SetMaterial` (`Character.Mesh` _asbp_character_template) 0 "/Game/_Guards/Art/Materials/PolygonMaster/M_Polygon_Inst_Dungeon01_CharactersRed.M_Polygon_Inst_Dungeon01_CharactersRed"))))))

(event `OnKO_Event`
  (params (Character :type "/Game/Blueprints/Core/BP_Character_Template Object Reference"))
  (`KismetSystemLibrary.Delay` 0.6)
  (`self.Drop`)
  (`self.Server Explode` (`self.K2_GetActorLocation`)))

(event `OnGameplayTagChange_Event`
  (params (GameplayTag :type "GameplayTag Structure") (NewTagCount :type Integer))
  (if (== GameplayTag (struct :`TagName` "Ability.Attack.Combo"))
    (`self.Drop`)
    (`self.Server Explode` (`self.K2_GetActorLocation`))))

(fn `UserConstructionScript`
  (`parent.UserConstructionScript`))