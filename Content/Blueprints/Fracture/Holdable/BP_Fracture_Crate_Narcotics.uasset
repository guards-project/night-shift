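; Fracturable, holdable narcotics crate that hops around on its own and drugs players caught in its explosion.
; Until fractured, the server repeatedly applies random impulse and torque with a giggle sound.
; Exploding spawns cosmetic Niagara and volumetric smoke, while a briefly enabled server overlap sphere applies a gameplay effect once per player.
; Physics updates wait for a local pawn unless forced, and equipping ignores physics-body collision to prevent launching.
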(event `self.ReceiveBeginPlay`
  (`parent.ReceiveBeginPlay`)
  (`/Engine/EditorBlueprintResources/ActorMacros.Switch Has Authority`
    (:`Authority`
      (`self.Bounce`))))

(event `self.On Equipped`
  (params (NewOwner :type "Actor Object Reference"))
  ;[1 1 1] stops flying into sky
  (`parent.On Equipped` NewOwner)
  (`PrimitiveComponent.SetCollisionResponseToChannel` (`self.Item Mesh`) "ECC_PhysicsBody" "ECR_Ignore"))

(event `Bounce`
  (bind _item_mesh (`self.Item Mesh`))
  (if (not (`self.Is Fractured`))
    (if (`SceneComponent.IsAnySimulatingPhysics` (`self.Item Mesh`))
      (`PrimitiveComponent.AddImpulse` _item_mesh (* (`KismetMathLibrary.MakeVector` (.x (`KismetMathLibrary.RandomUnitVector`)) (.y (`KismetMathLibrary.RandomUnitVector`)) (`KismetMathLibrary.RandomFloatInRange` 0.2 1.0)) (`KismetMathLibrary.RandomFloatInRange` 100.0 400.0)) "None" true)
      (`PrimitiveComponent.AddTorqueInDegrees` _item_mesh (* (`KismetMathLibrary.RandomUnitVector`) (`KismetMathLibrary.RandomFloatInRange` 3000.0 9000.0)) "None" true))
    (`self.MC hehe`)
    (`KismetSystemLibrary.Delay` (`KismetMathLibrary.RandomFloatInRange` 2.0 5.0))
    (`self.Bounce`)))

(event `self.On Unequipped`
  ;[1 1 1] stops flying into sky
  (`parent.On Unequipped`)
  (`PrimitiveComponent.SetCollisionResponseToChannel` (`self.Item Mesh`) "ECC_PhysicsBody" "ECR_Block"))

(event `MC hehe`
  (`GameplayStatics.PlaySoundAtLocation` "/Game/_Guards/Audio/Sounds/A_FairyEscape_Cue.A_FairyEscape_Cue" (`SceneComponent.K2_GetComponentLocation` (`self.Item Mesh`)) (struct) 0.05 1.0 0.0 null null null null))

(event `self.Enable Chaos`
  (`parent.Enable Chaos`)
  (`/Engine/EditorBlueprintResources/StandardMacros.DoOnce` false
    (:`Completed`
      (`ActorComponent.Deactivate` (`self.Niagara`))
      (`ActorComponent.Deactivate` (`self.Niagara1`)))))

(event `self.Server Explode`
  (params (Location :type "Vector Structure"))
  (`parent.Server Explode` Location)
  (`/Engine/EditorBlueprintResources/StandardMacros.DoOnce` false
    (:`Completed`
      (`/Engine/EditorBlueprintResources/ActorMacros.Switch Has Authority`
        (:`Authority`
          (`SceneComponent.K2_SetWorldLocation` (`self.Sphere`) Location false false)
          (`PrimitiveComponent.SetCollisionEnabled` (`self.Sphere`) "QueryOnly")
          (`KismetSystemLibrary.Delay` 0.5)
          (`PrimitiveComponent.SetCollisionEnabled` (`self.Sphere`) "NoCollision"))))))

(event `self.Set Mesh Highlight`
  (params (Show :type Boolean)))

(event `self.Set White Fill`
  (params (`White Fill Enabled` :type Boolean)))

(event `self.MC Explode`
  (params (Location :type "Vector Structure"))
  (`parent.MC Explode` Location)
  (`/Engine/EditorBlueprintResources/StandardMacros.DoOnce` false
    (:`Completed`
      (`/Engine/EditorBlueprintResources/StandardMacros.Can Execute Cosmetic Events`
        (:`True`
          (`NiagaraFunctionLibrary.SpawnSystemAtLocation` "/Game/TrailEffect/Fx/Niagara/NS_MiffExplosion.NS_MiffExplosion" Location)
          (bind _returnvalue (`|SpawnActorFromClass` "/Game/UltraVolumetrics/Blueprints/BP_UltraVolumetrics_Miff.BP_UltraVolumetrics_Miff_C" (`KismetMathLibrary.MakeTransform` Location) "Undefined" "MultiplyWithRoot" null "NewEnumerator0" 5.0 true 21.038341 -1.071999 3.277114 0.380952 (0.5 0.5 1.0) 2.0 1.0 (struct :`R` 0.739998 :`G` 0.499892 :`B` 1.0 :`A` 1.0) (struct :`R` 0.079448 :`G` 0.041378 :`B` 0.083333 :`A` 1.0) 0.0 0.0 -0.2 0.0 6000.0 1.612889 false 0.0 1.737688 0.180952 0.5 null))
          (`self.SetLifeSpan` _returnvalue 4.0))))))

(event `self.Sphere.OnComponentBeginOverlap`
  (params (OverlappedComponent :type "PrimitiveComponent Object Reference") (OtherActor :type "Actor Object Reference") (OtherComp :type "PrimitiveComponent Object Reference") (OtherBodyIndex :type Integer) (bFromSweep :type Boolean) (SweepResult :type "HitResult Structure (by ref)"))
  (bind _asbp_character_template_player (cast `/Game/Blueprints/Core/BP_Character_Template_Player` OtherActor))
  (if (not (`KismetArrayLibrary.Array_Contains` (`self.Drugged`) _asbp_character_template_player))
    (`KismetArrayLibrary.Array_AddUnique` (`self.Drugged`) _asbp_character_template_player)
    (bind _returnvalue (`AbilitySystemBlueprintLibrary.GetAbilitySystemComponent` _asbp_character_template_player))
    (`AbilitySystemComponent.BP_ApplyGameplayEffectToSelf` _returnvalue (`self.Gameplay Effect Class`) 6.0 (`AbilitySystemComponent.MakeEffectContext` _returnvalue))))

(event `self.Update Physics`
  (bind _returnvalue (`GameplayStatics.GetPlayerController` 0))
  ;[1 1 1] this fixes an issue where physics crates fall from dungeons before they are loaded
  ; call this when the client has spawned into the level
  (if (`self.Physics Enabled`)
    (`/Engine/EditorBlueprintResources/StandardMacros.IsValid` _returnvalue
      (:`Is Valid`
        (`/Engine/EditorBlueprintResources/StandardMacros.IsValid` (`Controller.K2_GetPawn` _returnvalue)
          (:`Is Valid`
            (`parent.Update Physics` :!label _label)))))
    (else
      (`parent.Update Physics`))))

(event `Force Update Physics`
  ;[1 1 1] this fixes an issue where physics crates fall from dungeons before they are loaded
  ; call this when the client has spawned into the level
  (goto _label))

(fn `Set Last Owner Glow`
  (params (Glow :type Boolean))
  ;[1 1 1] always visible
  (if (`self.Is Fractured`)
    (`SceneComponent.SetHiddenInGame` (`self.LootBeam`) true false)
    (else
      (`SceneComponent.SetHiddenInGame` (`self.LootBeam`) (`KismetSystemLibrary.IsValid` (`self.GetOwner`)) false))))

(fn `UserConstructionScript`
  (`parent.UserConstructionScript`))