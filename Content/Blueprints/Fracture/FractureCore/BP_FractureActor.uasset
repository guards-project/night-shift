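; Breakable, throwable item that swaps its static mesh for a Chaos Geometry Collection when fractured, making noise and spawning loot.
; Filtered damage above a threshold, throw impacts or airborne ragdoll hits fracture it via a spawned force actor, with IsFractured's OnRep enabling physics.
; Kick damage instead launches the collection when kick force is set, crediting the kicker with score.
; When a kicked piece breaks, it damages nearby targets and can knock out characters.
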(event `self.ReceiveBeginPlay`
  ;[1 1 1] Start
  (`parent.ReceiveBeginPlay`)
  (`self.Update Item Mesh Visibility` (or (`self.Geo Visible On Start`) (`self.Is Fractured`))))

(event `self.ReceiveRadialDamage`
  (params (DamageReceived :type "Float (single-precision)") (DamageType :type "DamageType Object Reference") (Origin :type "Vector Structure") (HitInfo :type "HitResult Structure (by ref)") (InstigatedBy :type "Controller Object Reference") (DamageCauser :type "Actor Object Reference"))
  ;[1 1 1] Damage Events
  (`self.On Damage` DamageReceived DamageType (* (`.Normal` (`GameplayStatics.BreakHitResult` HitInfo)) -1.0) Origin InstigatedBy DamageCauser))

(event `self.ReceivePointDamage`
  (params (Damage :type "Float (single-precision)") (DamageType :type "DamageType Object Reference") (HitLocation :type "Vector Structure") (HitNormal :type "Vector Structure") (HitComponent :type "PrimitiveComponent Object Reference") (BoneName :type Name) (ShotFromDirection :type "Vector Structure") (InstigatedBy :type "Controller Object Reference") (DamageCauser :type "Actor Object Reference") (HitInfo :type "HitResult Structure (by ref)"))
  ;[1 1 1] Damage Events
  (`self.On Damage` Damage DamageType ShotFromDirection HitLocation InstigatedBy DamageCauser))

(event `Kicked`
  (params (Direction :type "Vector Structure") (Location :type "Vector Structure") (Causer :type "Actor Object Reference"))
  ;[1 1 1] Launch the static mesh, only happens if launch is >0
  (`self.Set Kicker` Causer)
  (`self.Enable Chaos`)
  (`self.Add Geometry Impulse` Direction Location)
  (`self.KickEvent` self))

(event `Blink Collision`
  (bind _geometrycollection (`self.GeometryCollection`))
  (bind _geometrycollection_2 (`self.GeometryCollection`))
  ;[1 1 1] Test
  (`PrimitiveComponent.SetCollisionResponseToChannel` _geometrycollection_2 "ECC_WorldStatic" "ECR_Ignore")
  (`PrimitiveComponent.SetCollisionResponseToChannel` _geometrycollection_2 "ECC_WorldDynamic" "ECR_Ignore")
  (`KismetSystemLibrary.Delay` 0.1)
  (`PrimitiveComponent.SetCollisionResponseToChannel` _geometrycollection "ECC_WorldStatic" "ECR_Block")
  (`PrimitiveComponent.SetCollisionResponseToChannel` _geometrycollection "ECC_WorldDynamic" "ECR_Block"))

(event `Enable Chaos`
  (bind _geometrycollection (`self.GeometryCollection`))
  ;[1 1 1] Launch the static mesh, only happens if launch is >0
  (`|ExecutionSequence`
    (:`then_0`
      (`self.Update Item Mesh Visibility` true)
      (`|ExecutionSequence`
        (:`then_0`
          (`PrimitiveComponent.SetSimulatePhysics` (`self.Item Mesh`) false)
          (`PrimitiveComponent.SetCollisionEnabled` (`self.Item Mesh`) "NoCollision")
          (set `self.Idle Collision` "NoCollision")
          (set `self.Can Ever Interact` false))
        (:`then_1`
          (if (not (`SceneComponent.IsAnySimulatingPhysics` _geometrycollection))
            (`PrimitiveComponent.SetCollisionEnabled` (`self.GeometryCollection`) "PhysicsOnly")
            (`SceneComponent.K2_DetachFromComponent` (`self.GeometryCollection`) "KeepWorld" "KeepWorld" "KeepWorld" true)
            (`PrimitiveComponent.SetSimulatePhysics` _geometrycollection true)
            (`PrimitiveComponent.WakeAllRigidBodies` (`self.GeometryCollection`))))))
    (:`then_1`
      (`/Engine/EditorBlueprintResources/ActorMacros.Switch Has Authority`
        (:`Authority`
          (set `self.bCanBeDamaged` false))))
    (:`then_2`
      (`KismetSystemLibrary.Delay` 0.2)
      (`self.Set Last Owner Glow` false))))

(event `Set Kicker`
  (params (Causer :type "Actor Object Reference"))
  (bind _kicker (`self.Kicker`))
  ;[1 1 1] Launch the static mesh, only happens if launch is >0
  (bind _ascharacter (cast `Character` Causer))
  (set `self.Kicker` _ascharacter)
  (`|ExecutionSequence`
    (:`then_0`
      (`/Engine/EditorBlueprintResources/ActorMacros.Switch Has Authority`
        (:`Authority`
          (bind _playerstate (`Pawn.PlayerState` (`self.Kicker`))
            (:`then`
              (`/Game/Blueprints/Core/Score/BPFL_Score.Add Score` (`PlayerState.GetPlayerName` _playerstate) "Collateral" (`self.Score`)))
            (:`else`)))))
    (:`then_1`
      (`self.K2_AddActorLocalOffset` _kicker (-50.0 0.0 0.0) true false)
      (`self.K2_AddActorWorldOffset` (+ (* (`self.GetActorForwardVector` _kicker) 40.0) (0.0 0.0 10.0))))))

(event `self.Update Physics`
  ;[1 1 1] Launch the static mesh, only happens if launch is >0
  (if (`self.Is Fractured`)
    (`PrimitiveComponent.SetSimulatePhysics` (`self.Item Mesh`) false)
    (`PrimitiveComponent.SetCollisionEnabled` (`self.Item Mesh`) "NoCollision")
    (else
      (`parent.Update Physics`))))

(event `Server Explode`
  (params (Location :type "Vector Structure"))
  ;[1 1 1] Explode and Call MC
  (`/Engine/EditorBlueprintResources/StandardMacros.DoOnce` false
    (:`Completed`
      (set `self.bCanBeDamaged` false)
      (set `self.Is Fractured` true)
      (`self.MC Explode` Location)
      (`/Game/Blueprints/Core/PolygonAI/SenseData/BPFL_Noise.Create Noise` self (`self.K2_GetActorLocation`) (`self.Explode Noise AI`))
      (`self.Drop`)
      (`KismetSystemLibrary.Delay` 0.3)
      (`/Game/Blueprints/LootSpawner/BP_LootSpawner_Component.Spawn Loot` (`self.BP_LootSpawner_Component`) Location))))

(event `MC Explode`
  (params (Location :type "Vector Structure"))
  ;[1 1 1] Explode and Call MC
  (`GameplayStatics.PlaySoundAtLocation` (`self.Fracture Sound`) Location (struct) 1.0 1.0 0.0 null null null null))

(event `Destroy Attached Actors`
  ;[1 1 1] Enable Chaos Geo Component
  (`/Engine/EditorBlueprintResources/ActorMacros.Switch Has Authority`
    (:`Authority`
      (for _array_element (`self.GetAttachedActors` true)
        (`self.K2_DestroyActor` _array_element)))))

(event `self.GeometryCollection.OnChaosBreakEvent`
  (params (BreakEvent :type "ChaosBreakEvent Structure (by ref)"))
  (bind ((`Location` _location)) (break `ChaosBreakEvent` BreakEvent))
  ;[1 1 1] Damage
  (`/Engine/EditorBlueprintResources/ActorMacros.Switch Has Authority`
    (:`Authority`
      (`/Engine/EditorBlueprintResources/StandardMacros.DoOnce` false
        (:`Completed`
          (`GeometryCollectionComponent.SetNotifyBreaks` (`self.GeometryCollection`) false)
          (`self.Server Explode` _location)
          (`self.Break Damage` _location)
          (set `self.bCanBeDamaged` false))))))

(event `Break Damage`
  (params (Start :type "Vector Structure"))
  (bind _returnvalue (`self.Get Offset Damage Location` Start))
  ;[1 1 1] Damage
  (`self.Kicker`
    (:`then`
      (bind (_outactors _returnvalue_2) (`KismetSystemLibrary.SphereOverlapActors` Start 150.0 (`|MakeArray` "ObjectTypeQuery3" "ObjectTypeQuery1" :!type "EObjectTypeQuery Enum")))
      (bind _outhits (`KismetSystemLibrary.SphereTraceMultiForObjects` _returnvalue _returnvalue (`KismetMathLibrary.SelectFloat` 150.0 30.0 _returnvalue_2) (`|MakeArray` "ObjectTypeQuery3" "ObjectTypeQuery2" :!type "EObjectTypeQuery Enum") false (`|MakeArray` (`self.Kicker`) :!type "Actor Object Reference")))
      (for _array_element _outhits
        (bind (_bblockinghit _binitialoverlap _time _distance _location _impactpoint _normal _impactnormal _physmat _hitactor) (`GameplayStatics.BreakHitResult` _array_element))
        (`GameplayStatics.ApplyPointDamage` _hitactor (`self.On Break Damage`) (* _impactnormal -1.0) _array_element (`self.Damage Instigator`) self (`self.On Break Damage Type`))
        (if (`self.Break can KO`)
          (bind _asbp_character_template (cast `/Game/Blueprints/Core/BP_Character_Template` _hitactor))
          (`/Game/Blueprints/Core/BP_Character_Template.Enter KO` _asbp_character_template)))
      (set `self.bCanBeDamaged` false))
    (:`else`)))

(event `Force Break`
  ;[1 1 1] Force that triggers fracture
  (`/Engine/EditorBlueprintResources/StandardMacros.DoOnce` false
    (:`Completed`
      (bind _fracture_force_class (`self.Fracture Force Class`)
        (:`then`
          (`|SpawnActorFromClass` _fracture_force_class (`KismetMathLibrary.MakeTransform` (`self.GetActorBounds` true) (`KismetMathLibrary.MakeRotFromZ` (`self.Hit Direction`))) "AlwaysSpawn" "SelectDefaultAtRuntime" null (`self.Fracture Force Magnitude`) null)
          (`PrimitiveComponent.SetSimulatePhysics` (`self.Item Mesh`) false)
          (`PrimitiveComponent.SetCollisionEnabled` (`self.Item Mesh`) "NoCollision")
          (`/Engine/EditorBlueprintResources/ActorMacros.Switch Has Authority`
            (:`Authority`
              (set `self.bCanBeDamaged` false))))
        (:`else`)))))

(event `self.Item Mesh.OnComponentHit`
  (params (HitComponent :type "PrimitiveComponent Object Reference") (OtherActor :type "Actor Object Reference") (OtherComp :type "PrimitiveComponent Object Reference") (NormalImpulse :type "Vector Structure") (Hit :type "HitResult Structure (by ref)"))
  ;[1 1 1] If hit by a dead or ko character that is in the air - then explode
  (bind _dead (message `/Game/Blueprints/Core/BPI_Character.Is Dead` OtherActor))
  (bind _ko (message `/Game/Blueprints/Core/BPI_Character.Is KO` OtherActor))
  (if (or _dead _ko)
    (if (>= (`KismetMathLibrary.VSize` (`SceneComponent.GetComponentVelocity` OtherComp)) 150.0)
      (bind (_outhit _returnvalue) (`/Game/Blueprints/Core/BPFL_Guards.Is Component On Ground` OtherComp (`|MakeArray` OtherActor self :!type "Actor Object Reference") "Persistent"))
      (if (not _returnvalue)
        (`GameplayStatics.ApplyPointDamage` self 100.0 NormalImpulse Hit null OtherActor "/Game/Blueprints/Items/DamageTypes/DamageType_Polygon.DamageType_Polygon_C")))))

(fn `Add Geometry Impulse`
  (params (InVec :type "Vector3f Structure") (Location :type "Vector Structure"))
  (bind (_x _y _z) (`KismetMathLibrary.BreakVector3f` InVec))
  (bind _geometrycollection (`self.GeometryCollection`))
  (bind _returnvalue (`KismetMathLibrary.MakeVector` _x _y (`KismetMathLibrary.FMax` _z (`self.Kick Lift`))))
  (`PrimitiveComponent.AddImpulse` _geometrycollection (* _returnvalue (`self.Kick Force`)) "None" true)
  (`PrimitiveComponent.AddForceAtLocation` _geometrycollection (* _returnvalue (`self.Kick Spin`)) Location "None"))

(fn `Anchor Bounds`
  ;[1 1 1] TODO - bounds calculator using widget-like anchor locations
  (`AddComponent|NODE_AddChildActorComponent-0`))

(fn `Apply Thrown Damage`
  (`parent.Apply Thrown Damage`)
  (`self.Server Explode` (`self.K2_GetActorLocation`))
  ;[1 1 1] Also radial
  (`GameplayStatics.ApplyRadialDamage` :`BaseDamage` (`self.Hit Damage`) :`Origin` (`self.K2_GetActorLocation`) :`DamageRadius` (`self.Hit Damage Radius`) :`DamageTypeClass` (`self.Hit Damage Type Class`) :`DamageCauser` self :`InstigatedByController` (`self.Get Damage Instigator`) :`bDoFullDamage` true :`DamagePreventionChannel` "ECC_Camera") ; create radial damage\nwhich causes fracture, and others in location (such as enemy hit)\nif self is set as causer, it does not damage self
)

(fn `Get Can Interact`
  (returns (ReturnValue :type Boolean))
  (bind _returnvalue (`parent.Get Can Interact`))
  (return (and _returnvalue (not (`self.Is Fractured`)))))

(fn `Get Offset Damage Location`
  (params (Location :type "Vector Structure"))
  (returns (ReturnValue :type "Vector Structure"))
  (bind _kicker (`self.Kicker`)
    (:`then`
      (return (+ (* (`KismetMathLibrary.GetDirectionUnitVector` (`self.K2_GetActorLocation` _kicker) (`local.Location`)) 100.0) (`local.Location`))))
    (:`else`
      (return Location))))

(fn `On Damage`
  (params (`In Damage` :type "Float (single-precision)") (`In Damage Type` :type "DamageType Object Reference") (`In Direction` :type "Vector Structure") (`In Location` :type "Vector Structure") (`In Instigator` :type "Controller Object Reference") (`In Causer` :type "Actor Object Reference"))
  (bind _explicit_damage_types (`self.Explicit Damage Types`))
  (if (`self.bCanBeDamaged`)
    (if (or (`KismetArrayLibrary.Array_IsEmpty` _explicit_damage_types) (`KismetArrayLibrary.Array_Contains` _explicit_damage_types (`GameplayStatics.GetObjectClass` `In Damage Type`)))
      (if (>= (`local.In Damage`) (`self.Damage Threshold`))
        (set `self.Damage Instigator` (`local.In Instigator`))
        (if (and (> (`self.Kick Force`) 0.0) (== (`GameplayStatics.GetObjectClass` (`local.In Damage Type`)) "/Game/Blueprints/Items/DamageTypes/DamageType_Polygon_Kick.DamageType_Polygon_Kick_C"))
          (`self.Kicked` (`local.In Direction`) (`local.In Location`) (`local.In Causer`))
          (else
            (`self.Server Explode` (`self.K2_GetActorLocation`))
            (set `self.Hit Direction` (`local.In Direction`))
            (`self.Force Break`)))
        (set `self.bCanBeDamaged` false)))))

(fn `OnRep_Is Fractured`
  (if (`self.Is Fractured`)
    (`self.Enable Chaos`)
    (`self.Force Break`)
    (set `self.Can Ever Interact` false)
    (`self.Fractured` self)))

(fn `Set Last Owner Glow`
  (params (Glow :type Boolean))
  ;[1 1 1] always visible
  (if (`self.Is Fractured`)
    (`SceneComponent.SetHiddenInGame` (`self.LootBeam`) true false)
    (else
      (`parent.Set Last Owner Glow` Glow))))

(fn `Update Item Mesh Visibility`
  (params (`Geo Visible` :type Boolean))
  (if `Geo Visible`
    (`SceneComponent.SetVisibility` (`self.Item Mesh`) false false)
    (`SceneComponent.SetVisibility` (`self.GeometryCollection`) true false)
    (else
      (`SceneComponent.SetVisibility` (`self.Item Mesh`) true false)
      (`SceneComponent.SetVisibility` (`self.GeometryCollection`) false false))))

(fn `UserConstructionScript`
  (`parent.UserConstructionScript`))