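; Work-in-progress destructible actor that launches a Chaos geometry collection when hit by point damage.
; A Blocker box, sized to the mesh bounds, drops its collision on a hit or when Fractured replicates.
; Damage enables physics, applies upward-clamped force and impulse along the shot direction, and nudges the damage causer back.
; The debris collision handler only checks authority; its knock-on damage logic is disconnected.
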(event `self.ReceiveBeginPlay`
  ;[1 1 1] wip
  (`self.Init Blocker`))

(event `self.ReceivePointDamage`
  (params (Damage :type "Float (single-precision)") (DamageType :type "DamageType Object Reference") (HitLocation :type "Vector Structure") (HitNormal :type "Vector Structure") (HitComponent :type "PrimitiveComponent Object Reference") (BoneName :type Name) (ShotFromDirection :type "Vector Structure") (InstigatedBy :type "Controller Object Reference") (DamageCauser :type "Actor Object Reference") (HitInfo :type "HitResult Structure (by ref)"))
  (bind (_x _y _z) (`KismetMathLibrary.BreakVector3f` ShotFromDirection))
  (bind _geometrycollectioncomponent (`self.GeometryCollectionComponent`))
  (bind _geometrycollectioncomponent_2 (`self.GeometryCollectionComponent`))
  (bind _returnvalue (`KismetMathLibrary.MakeVector` _x _y (`KismetMathLibrary.FMax` _z 0.1)))
  ;[1 1 1] wip
  (`self.K2_AddActorLocalOffset` DamageCauser (-100.0 0.0 0.0) true false)
  (set `self.Damage Instigator` InstigatedBy)
  (`PrimitiveComponent.SetCollisionEnabled` (`self.Blocker`) "NoCollision")
  (`PrimitiveComponent.IgnoreActorWhenMoving` _geometrycollectioncomponent_2 DamageCauser true)
  (`PrimitiveComponent.SetSimulatePhysics` _geometrycollectioncomponent_2 true)
  (`PrimitiveComponent.WakeAllRigidBodies` (`self.GeometryCollectionComponent`))
  (`PrimitiveComponent.AddForceAtLocation` _geometrycollectioncomponent (* _returnvalue 10000000.0) HitLocation "None")
  (`PrimitiveComponent.AddImpulse` _geometrycollectioncomponent (* _returnvalue 500.0) "None" true))

(event `self.GeometryCollectionComponent.OnChaosPhysicsCollision`
  (params (CollisionInfo :type "ChaosPhysicsCollisionInfo Structure (by ref)"))
  ;[1 1 1] wip
  (`/Engine/EditorBlueprintResources/ActorMacros.Switch Has Authority`))

(fn `Init Blocker`
  (bind _blocker (`self.Blocker`))
  (bind (_returnvalue_origin _returnvalue_boxextent) (`KismetMathLibrary.BreakBoxSphereBounds` (`StaticMesh.GetBounds` (`self.Mesh`))))
  (`BoxComponent.SetBoxExtent` _blocker _returnvalue_boxextent true)
  (`SceneComponent.K2_SetRelativeLocation` _blocker _returnvalue_origin false false))

(fn `OnRep_Fractured`
  (`PrimitiveComponent.SetCollisionEnabled` (`self.Blocker`) "NoCollision"))

(fn `UserConstructionScript`
  (`self.Init Blocker`))