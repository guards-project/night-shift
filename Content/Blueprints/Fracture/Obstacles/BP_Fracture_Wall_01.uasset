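; BP_Fracture_Wall_01 is a fracturable wall obstacle built on a Geometry Collection, extending a parent that handles server-side explosions.
; Its construction script registers anchor field actors from child actor components as initialization fields on the Geometry Collection.
; On ServerExplode it calls the parent, then once only resets the nav modifier's area class with no class specified, changing navigation at the wall.
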(event `self.Server Explode`
  (params (Location :type "Vector Structure"))
  (`parent.Server Explode` Location)
  (`/Engine/EditorBlueprintResources/StandardMacros.DoOnce` false
    (:`Completed`
      (`NavModifierComponent.SetAreaClass` (`self.NavModifier`) null))))

(fn `UserConstructionScript`
  (`parent.UserConstructionScript`)
  (for _array_element (`self.K2_GetComponentsByClass` "/Script/Engine.ChildActorComponent")
    (bind _asfs_anchor_field_generic (cast `/Engine/EditorResources/FieldNodes/FS_AnchorField_Generic` (`ChildActorComponent.ChildActor` _array_element)))
    (`KismetArrayLibrary.Array_Add` (`GeometryCollectionComponent.InitializationFields` (`self.GeometryCollection`)) _asfs_anchor_field_generic)))