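; Interactable cape pickup that unlocks a cosmetic cape for the local player who uses it.
; The construction script maps its ID to a DT_Capes row, setting the mesh and synchronously loaded material.
; BeginPlay destroys it if the "Cosmetic" save already lists that row as purchased.
; Interacting fires a UMG event, unlocks the row through the pawn's BP_Cosmetic_Component save, then destroys the actor.
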(event `self.ReceiveBeginPlay`
  (bind _returnvalue (`GameplayStatics.DoesSaveGameExist` "Cosmetic"))
  (if _returnvalue
    (bind _returnvalue_2 (`GameplayStatics.LoadGameFromSlot` "Cosmetic"))
    (bind _assave_game_cosmetics (cast `/Game/Blueprints/Customisation/SaveGame_Cosmetics` _returnvalue_2))
    (if (`KismetArrayLibrary.Array_Contains` (`/Game/Blueprints/Customisation/SaveGame_Cosmetics.Purchased Rows` _assave_game_cosmetics) (`self.Row`))
      (`self.K2_DestroyActor`))))

(event `/Game/Primer/Primer_Interaction/BPI_Interact.Execute Interact`
  (params (User :type "Controller Object Reference"))
  (`/Engine/EditorBlueprintResources/StandardMacros.IsValid` User
    (:`Is Valid`
      (if (`Controller.IsLocalController` User)
        (`/Game/Primer/Primer_UMGEvent/BPFL_Primer_UMGEvent.Create UMG Event` (`self.UMG Event`))
        (`/Game/Blueprints/Customisation/SaveGame_Cosmetics.Unlock Cosmetic` (`/Game/Blueprints/Customisation/BP_Cosmetic_Component.Save` (`self.GetComponentByClass` (`Controller.K2_GetPawn` User) "/Game/Blueprints/Customisation/BP_Cosmetic_Component.BP_Cosmetic_Component_C")) (`self.Row`))
        (`self.K2_DestroyActor`)))))

(fn `Update Cape`
  (locals (`L Default Cape` :type "Object Soft Object Reference" :default "/Game/PolygonFantasyKingdom/Meshes/Chr/Attach/SK_Chr_King_Cape_01.SK_Chr_King_Cape_01"))
  (bind _outrownames (`DataTableFunctionLibrary.GetDataTableRowNames` "/Game/Blueprints/Customisation/Capes/DT_Capes.DT_Capes"))
  (bind _output (`|GetArrayItem` _outrownames (`KismetMathLibrary.Conv_ByteToInt` (`self.ID`))))
  (set `self.Row` (make `DataTableRowHandle` "/Game/Blueprints/Customisation/Capes/DT_Capes.DT_Capes" _output))
  (bind _returnvalue (`|GetDataTableRow` "/Game/Blueprints/Customisation/Capes/DT_Capes.DT_Capes" _output)
    (:`then`
      (bind (_cape _mat) (break `/Game/Blueprints/Customisation/Capes/F_Cape` _returnvalue))
      (`StaticMeshComponent.SetStaticMesh` (`self.SM_Cape`) (select `bool` (== _cape (`local.L Default Cape`)) :`false` "/Game/Blueprints/Customisation/Capes/SM_FancyCape.SM_FancyCape" :`true` "/Game/Blueprints/Customisation/Capes/SM_Cape.SM_Cape" :!type "StaticMesh Object Reference"))
      (bind _returnvalue_2 (`KismetSystemLibrary.LoadAsset_Blocking` _mat))
      (bind _asmaterial_interface (cast `MaterialInterface` _returnvalue_2))
      (`PrimitiveComponent.SetMaterial` (`self.SM_Cape`) 0 _asmaterial_interface))))

(fn `UserConstructionScript`
  (`parent.UserConstructionScript`)
  (`self.Update Cape`))