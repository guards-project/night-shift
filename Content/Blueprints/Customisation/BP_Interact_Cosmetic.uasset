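; Interactable cosmetics station that opens the W_Cosmetics menu for the local player who uses it.
; On interact it pushes the widget, switches the character to third person, and enters cinematic mode to lock movement and turning.
; It teleports the player in front of the station on server and client, aligning rotation and camera.
; A flag re-armed on widget deactivation and a viewport check on the cached widget gate reuse.
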(event `/Game/Primer/Primer_Interaction/BPI_Interact.Execute Interact`
  (params (User :type "Controller Object Reference"))
  (bind _returnvalue (`GameplayStatics.GetPlayerController` 0))
  (bind (_returnvalue_roll _returnvalue_pitch _returnvalue_yaw) (`KismetMathLibrary.BreakRotator` (`self.K2_GetActorRotation`)))
  (bind (_returnvalue_roll_2 _returnvalue_pitch_2 _returnvalue_yaw_2) (`KismetMathLibrary.BreakRotator` (`self.K2_GetActorRotation`)))
  (bind _returnvalue_2 (+ (`self.K2_GetActorLocation`) (* (`self.GetActorForwardVector`) 100.0)))
  (`parent.Execute Interact` User)
  (`/Engine/EditorBlueprintResources/StandardMacros.IsValid` User
    (:`Is Valid`
      (if (`Controller.IsLocalPlayerController` User)
        (if (`self.Can Draw`)
          (set `self.Can Draw` false)
          (bind (_commonstack _stack_menu) (`/Game/_Guards/UserInterface/Menus/Stack/BPFL_CommonStack.Push Menu` "/Game/Blueprints/Customisation/UI/W_Cosmetics.W_Cosmetics_C"))
          (`KismetSystemLibrary.Delay` 0.2)
          (bind _returnvalue_3 (`CommonActivatableWidgetContainerBase.GetActiveWidget` _stack_menu))
          (bind _asw_cosmetics (cast `/Game/Blueprints/Customisation/UI/W_Cosmetics` _returnvalue_3))
          (set `self.Cosmetic Widget` _asw_cosmetics)
          (add `CommonActivatableWidget.BP_OnWidgetDeactivated` _returnvalue_3 (delegate `BP_OnWidgetDeactivated_Event`))
          (bind _asbp_character_template_player (cast `/Game/Blueprints/Core/BP_Character_Template_Player` (`GameplayStatics.GetPlayerPawn` 0)))
          (`/Game/Blueprints/Core/BP_Character_Template_Player.Set Third Person` _asbp_character_template_player true)
          (`|ExecutionSequence`
            (:`then_0`
              (`/Game/Blueprints/Core/BP_Character_Template.Server Set Move State` _asbp_character_template_player "NewEnumerator0")
              (`/Game/Blueprints/Core/BP_Character_Template_Player.Set Zoom Level` _asbp_character_template_player 0)
              (`self.K2_SetActorRotation` _asbp_character_template_player (`KismetMathLibrary.MakeRotator` 0.0 0.0 _returnvalue_yaw) false)
              (`Controller.SetControlRotation` _returnvalue (`KismetMathLibrary.MakeRotator` (.roll (`Controller.GetControlRotation` _returnvalue)) -10.0 (+ _returnvalue_yaw_2 180.0)))
              (`PlayerController.SetCinematicMode` _returnvalue true false false true true)
              (bind _asbp_player_controller_template (cast `/Game/Blueprints/Core/BP_PlayerController_Template` (`GameplayStatics.GetPlayerController` 0)))
              (`/Game/Blueprints/Core/BP_PlayerController_Template.Server Set Location` _asbp_player_controller_template _returnvalue_2)
              (`self.K2_SetActorLocation` (`Controller.K2_GetPawn` (`GameplayStatics.GetPlayerController` 0)) _returnvalue_2 false false))
            (:`then_1`
              (`KismetSystemLibrary.Delay` 0.0)
              (set `SpringArmComponent.SocketOffset` (0.0 0.0 -30.0) (`/Game/Blueprints/Core/BP_Character_Template_Player.SpringArm` _asbp_character_template_player)))))))))

(event `BP_OnWidgetDeactivated_Event`
  (set `self.Can Draw` true))

(fn `Get Can Interact`
  (returns (ReturnValue :type Boolean))
  (bind _cosmetic_widget (`self.Cosmetic Widget`)
    (:`then`
      (return (not (`Widget.IsInViewport` _cosmetic_widget))))
    (:`else`
      (return true))))

(fn `UserConstructionScript`
  (`parent.UserConstructionScript`))