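; Armor stand actor that mirrors the local player's cosmetics and equipped shield as a display.
; On BeginPlay, where cosmetics can run, it binds to the pawn's cosmetic and inventory components, retrying by timer until a pawn exists.
; Cosmetic updates build or reuse one skeletal mesh per data table, socket-attached or leader-posed, then apply skin, armor colors and cape.
; Shield changes copy the offhand item's mesh; cosmetic assets load synchronously.
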(event `self.ReceiveBeginPlay`
  (`KismetSystemLibrary.Delay` 0.1)
  (`/Engine/EditorBlueprintResources/StandardMacros.Can Execute Cosmetic Events`
    (:`True`
      (`self.Bind to Cosmetics`)
      (`self.Bind to Shield`)
      (`self.SetActorEnableCollision` false))))

(event `Bind to Cosmetics`
  (bind _returnvalue (`Controller.K2_GetPawn` (`GameplayStatics.GetPlayerController` 0)))
  (`/Engine/EditorBlueprintResources/StandardMacros.IsValid` _returnvalue
    (:`Is Valid`
      (bind _output_get (set `self.Cosmetic Comp` (`self.GetComponentByClass` _returnvalue "/Game/Blueprints/Customisation/BP_Cosmetic_Component.BP_Cosmetic_Component_C")))
      (add `/Game/Blueprints/Customisation/BP_Cosmetic_Component.Data Updated` _output_get (delegate `Data Updated_Event`))
      (`self.Data Updated_Event`))
    (:`Is Not Valid`
      (`KismetSystemLibrary.K2_SetTimerDelegate` (delegate `Bind to Cosmetics`) 0.5))))

(event `Data Updated_Event`
  (bind _cape (`self.Cape`))
  (bind _cosmetic_comp (`self.Cosmetic Comp`))
  (bind _replicated_armor_colors (`/Game/Blueprints/Customisation/BP_Cosmetic_Component.Replicated Armor Colors` (`self.Cosmetic Comp`)))
  (bind _returnvalue (`KismetMathLibrary.Conv_LinearColorToVector` (`/Game/Blueprints/Customisation/BP_Cosmetic_Component.Skin Color` _cosmetic_comp)))
  (for _array_element (`/Game/Blueprints/Customisation/BP_Cosmetic_Component.Replicated Row Handles` _cosmetic_comp)
    (`self.Set Skeletal Mesh` _array_element))
  (bind _keys (`BlueprintMapLibrary.Map_Keys` (`self.Skeletal Meshes`)))
  (`MeshComponent.SetVectorParameterValueOnMaterials` _keys "Color_Skin" _returnvalue)
  (`MeshComponent.SetVectorParameterValueOnMaterials` _keys "Color_Stubble" (* _returnvalue 0.7))
  (bind _keys_2 (`BlueprintMapLibrary.Map_Keys` (`self.Skeletal Meshes`)))
  (for (_array_element_2 _array_index) _keys_2
    (bind _returnvalue_2 (`KismetMathLibrary.Min` _array_index (`KismetArrayLibrary.Array_LastIndex` _replicated_armor_colors)))
    (if (`KismetArrayLibrary.Array_IsValidIndex` _replicated_armor_colors _returnvalue_2)
      (`self.Apply Armor Params` (`|GetArrayItem` _replicated_armor_colors _returnvalue_2) _array_element_2)))
  (bind _outrownames (`DataTableFunctionLibrary.GetDataTableRowNames` "/Game/Blueprints/Customisation/Capes/DT_Capes.DT_Capes"))
  (bind _returnvalue_3 (`|GetDataTableRow` "/Game/Blueprints/Customisation/Capes/DT_Capes.DT_Capes" (`|GetArrayItem` _outrownames (`KismetMathLibrary.Conv_ByteToInt` (`/Game/Blueprints/Customisation/BP_Cosmetic_Component.Cape ID` (`self.Cosmetic Comp`)))))
    (:`then`
      (`|ExecutionSequence`
        (:`then_0`
          (bind (_cape_2 _mat) (break `/Game/Blueprints/Customisation/Capes/F_Cape` _returnvalue_3))
          (if (`KismetSystemLibrary.IsValidSoftObjectReference` _cape_2)
            (bind _returnvalue_4 (`KismetSystemLibrary.LoadAsset_Blocking` _cape_2))
            (bind _asskeletal_mesh (cast `SkeletalMesh` _returnvalue_4))
            (`SkeletalMeshComponent.SetSkeletalMeshAsset` _cape _asskeletal_mesh)
            (else
              (`SkeletalMeshComponent.SetSkeletalMeshAsset` _cape null))))
        (:`then_1`
          (bind _returnvalue_5 (`KismetSystemLibrary.LoadAsset_Blocking` _mat))
          (bind _asmaterial_interface (cast `MaterialInterface` _returnvalue_5))
          (`PrimitiveComponent.SetMaterial` _cape 0 _asmaterial_interface))
        (:`then_2`
          (`SceneComponent.SetVisibility` (`self.Cape`) true false))))))

(event `Bind to Shield`
  (bind _returnvalue (`Controller.K2_GetPawn` (`GameplayStatics.GetPlayerController` 0)))
  (bind _returnvalue_2 (`self.GetComponentByClass` _returnvalue "/Game/Blueprints/Items/BP_Inventory_Component.BP_Inventory_Component_C"))
  (`/Engine/EditorBlueprintResources/StandardMacros.IsValid` _returnvalue
    (:`Is Valid`
      (add `/Game/Blueprints/Items/BP_Inventory_Component.OnEquippedItemChanged` _returnvalue_2 (delegate `OnEquippedItemChanged_Event`))
      (bind (_item _shield) (`/Game/Blueprints/Items/BP_Inventory_Component.Get Items` _returnvalue_2))
      (`self.OnEquippedItemChanged_Event` null _shield))
    (:`Is Not Valid`
      (`KismetSystemLibrary.K2_SetTimerDelegate` (delegate `Bind to Shield`) 0.5))))

(event `OnEquippedItemChanged_Event`
  (params (Mainhand :type "/Game/Blueprints/Items/BP_Item Object Reference") (Offhand :type "/Game/Blueprints/Items/BP_Item Object Reference"))
  (`/Engine/EditorBlueprintResources/StandardMacros.IsValid` Offhand
    (:`Is Valid`
      (bind _asbp_shield_master (cast `/Game/Blueprints/Items/Shield/BP_Shield_Master` Offhand)
        (:`then`
          (`StaticMeshComponent.SetStaticMesh` (`self.Shield`) (`StaticMeshComponent.StaticMesh` (`/Game/Blueprints/Items/BP_Item.Item Mesh` _asbp_shield_master))))
        (:`CastFailed`
          (`StaticMeshComponent.SetStaticMesh` (`self.Shield`) null :!label _label))))
    (:`Is Not Valid`
      (goto _label))))

(fn `Apply Armor Params`
  (params (Color :type "/Game/Blueprints/Customisation/F_ArmorColor Structure") (Mesh :type "SkeletalMeshComponent Object Reference"))
  (bind (_color_primary _color_secondary _color_metal_primary _color_metal_secondary _color_metal_dark _color_leather_primary _color_leather_secondary) (break `/Game/Blueprints/Customisation/F_ArmorColor` (`local.Color`)))
  (`/Engine/EditorBlueprintResources/StandardMacros.IsValid` Mesh
    (:`Is Valid`
      (for (_array_element _array_index) (`|MakeArray` _color_primary _color_secondary _color_metal_primary _color_metal_secondary _color_metal_dark _color_leather_primary _color_leather_secondary)
        (`MeshComponent.SetVectorParameterValueOnMaterials` (`local.Mesh`) (`|GetArrayItem` (`|MakeArray` "Color_Primary" "Color_Secondary" "Color_Metal_Primary" "Color_Metal_Secondary" "Color_Metal_Dark" "Color_Leather_Primary" "Color_Leather_Secondary" :!type "Name") _array_index) (`KismetMathLibrary.Conv_LinearColorToVector` _array_element))))))

(fn `Set Skeletal Mesh`
  (params (DataTableRowHandle :type "DataTableRowHandle Structure (by ref)"))
  (returns (`Skeletal Mesh Comp` :type "SkeletalMeshComponent Object Reference"))
  (locals (`L Data` :type "/Game/Blueprints/Customisation/F_CosmeticDefinition Structure") (`L New Mesh` :type "SkeletalMesh Object Reference") (`L Skeletal Mesh Component` :type "SkeletalMeshComponent Object Reference"))
  (bind (_datatable _rowname) (break `DataTableRowHandle` DataTableRowHandle))
  (bind _skeletal_meshes (`self.Skeletal Meshes`))
  (bind _l_skeletal_mesh_component (`local.L Skeletal Mesh Component`))
  (bind _l_skeletal_mesh_component_2 (`local.L Skeletal Mesh Component`))
  (bind _skeletal_meshes_2 (`self.Skeletal Meshes`))
  (bind _l_skeletal_mesh_component_3 (`local.L Skeletal Mesh Component`))
  (bind _skeletalmesh (`self.SkeletalMesh`))
  (bind (_skelmesh _name _cost _socket _relativetransform) (break `/Game/Blueprints/Customisation/F_CosmeticDefinition` (`local.L Data`)))
  (bind (_skelmesh_2 _name_2 _cost_2 _socket_2 _relativetransform_2) (break `/Game/Blueprints/Customisation/F_CosmeticDefinition` (`local.L Data`)))
  ;[1 1 1] Cache new mesh to apply
  (`/Engine/EditorBlueprintResources/StandardMacros.Can Execute Cosmetic Events`
    (:`True`
      (`/Engine/EditorBlueprintResources/StandardMacros.IsValid` _datatable
        (:`Is Valid`
          (bind _returnvalue (`|GetDataTableRow` _datatable _rowname)
            (:`then`
              (set `local.L Data` _returnvalue)
              (bind _returnvalue_2 (`KismetSystemLibrary.LoadAsset_Blocking` (`.SkelMesh_12_8E7CDD4249BA3C60911401A0BE87031F` (break `/Game/Blueprints/Customisation/F_CosmeticDefinition` _returnvalue))))
              (bind _asskeletal_mesh (cast `SkeletalMesh` _returnvalue_2))
              (set `local.L New Mesh` _asskeletal_mesh))
            (:`RowNotFound`
              (bind _outrownames (`DataTableFunctionLibrary.GetDataTableRowNames` _datatable))
              (bind _returnvalue_3 (`|GetDataTableRow` _datatable (`|GetArrayItem` _outrownames))
                (:`then`
                  (bind _returnvalue_4 (`KismetSystemLibrary.LoadAsset_Blocking` (`.SkelMesh_12_8E7CDD4249BA3C60911401A0BE87031F` (break `/Game/Blueprints/Customisation/F_CosmeticDefinition` _returnvalue_3))))
                  (bind _asskeletal_mesh_2 (cast `SkeletalMesh` _returnvalue_4))
                  (set `local.L New Mesh` _asskeletal_mesh_2)))))
          (`local.L New Mesh`
            (:`then`
              ;[1 1 1] Find existing mesh for this data table and update it
              (bind _values (`BlueprintMapLibrary.Map_Values` _skeletal_meshes))
              (for (_array_element _array_index) _values
                (if (== (`.DataTable` (break `DataTableRowHandle` _array_element)) (`.DataTable` (break `DataTableRowHandle` (`local.DataTableRowHandle`))))
                  (bind _keys (`BlueprintMapLibrary.Map_Keys` _skeletal_meshes))
                  (set `local.L Skeletal Mesh Component` (`|GetArrayItem` _keys _array_index))
                  (`SkinnedMeshComponent.SetSkinnedAssetAndUpdate` _l_skeletal_mesh_component (`local.L New Mesh`) true)
                  (`BlueprintMapLibrary.Map_Remove` _skeletal_meshes_2 _l_skeletal_mesh_component)
                  (`BlueprintMapLibrary.Map_Add` _skeletal_meshes_2 _l_skeletal_mesh_component (`local.DataTableRowHandle`))
                  (`MeshComponent.SetVectorParameterValueOnMaterials` (`local.L Skeletal Mesh Component`) "Color_Skin" (`KismetMathLibrary.Conv_LinearColorToVector` (`/Game/Blueprints/Customisation/BP_Cosmetic_Component.Skin Color` (`self.Cosmetic Comp`))))
                  (`SceneComponent.K2_AttachToComponent` _l_skeletal_mesh_component_3 _skeletalmesh _socket "SnapToTarget" "SnapToTarget" "SnapToTarget" true)
                  (`SceneComponent.K2_SetRelativeTransform` _l_skeletal_mesh_component_3 _relativetransform false false)
                  (if (== _socket "None")
                    (`SkinnedMeshComponent.SetLeaderPoseComponent` (`local.L Skeletal Mesh Component`) _skeletalmesh false false))
                  (return (`local.L Skeletal Mesh Component`))))
              ;[1 1 1] Cannot find mapped skeletalmesh& data table combo - create new skeletal mesh
              (bind _returnvalue_5 (`|AddComponentByClass` "/Script/Engine.SkeletalMeshComponent"))
              (`BlueprintMapLibrary.Map_Add` (`self.Skeletal Meshes`) _returnvalue_5 (`local.DataTableRowHandle`))
              (set `SceneComponent.bUseAttachParentBound` true _returnvalue_5)
              (set `local.L Skeletal Mesh Component` _returnvalue_5)
              (`SkinnedMeshComponent.SetSkinnedAssetAndUpdate` (`local.L Skeletal Mesh Component`) (`local.L New Mesh`) true)
              (`SceneComponent.K2_AttachToComponent` (`local.L Skeletal Mesh Component`) (`self.SkeletalMesh`) _socket_2 "SnapToTarget" "SnapToTarget" "SnapToTarget" true)
              (`SceneComponent.K2_SetRelativeTransform` (`local.L Skeletal Mesh Component`) _relativetransform_2 false false)
              (if (== _socket_2 "None")
                (`SkinnedMeshComponent.SetLeaderPoseComponent` _l_skeletal_mesh_component_2 (`self.SkeletalMesh`) false false))
              (`PrimitiveComponent.SetCastHiddenShadow` _l_skeletal_mesh_component_2 true)
              (`PrimitiveComponent.SetCollisionEnabled` _l_skeletal_mesh_component_2 "NoCollision")
              (`ActorComponent.SetComponentTickEnabled` (`local.L Skeletal Mesh Component`) false)
              ;[1 1 1] Apply Dynamic Material
              (`MeshComponent.SetVectorParameterValueOnMaterials` (`local.L Skeletal Mesh Component`) "Color_Skin" (`KismetMathLibrary.Conv_LinearColorToVector` (`/Game/Blueprints/Customisation/BP_Cosmetic_Component.Skin Color` (`self.Cosmetic Comp`))))
              (return (`local.L Skeletal Mesh Component`)))
            (:`else`)))))))

(fn `UserConstructionScript`)