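; Character cosmetics component that saves and replicates a player's modular armor, armor colors, skin color and cape.
; The locally controlled owner loads SaveGame_Cosmetics and sends it to the server, and OnRep functions apply the replicated data.
; Each DataTable row handle drives one runtime skeletal mesh, socketed or leader-posed to the hidden body mesh and tinted through material parameters.
; It also supports previews and stencil outlines, and checks the guard armor achievement.
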(event `self.ReceiveBeginPlay`
  (`KismetSystemLibrary.Delay` 0.2)
  (`self.Init`))

(event `Init`
  (bind _returnvalue (`KismetSystemLibrary.K2_SetTimerDelegate` (`|CreateDelegate` :!event `Init`) 5.0))
  (set `self.Reload Fallback` _returnvalue)
  (bind _ascharacter (cast `Character` (`self.GetOwner`)))
  (`SceneComponent.SetVisibility` (`Character.Mesh` _ascharacter) false false)
  (if (`Pawn.IsLocallyControlled` _ascharacter)
    (set `self.Locally Owned` true)
    (`self.Load Save`)))

(event `Server Set Mesh`
  (params (Data :type "DataTableRowHandle Structure"))
  ;[1 1 1] Meshes
  (`self.Set Mesh` Data))

(event `Server Set All Meshes`
  (params (Data :type "Array of DataTableRowHandle Structure"))
  ;[1 1 1] Meshes
  (set `self.Replicated Row Handles` Data))

(event `Set Skin Color`
  (params (`Skin Color` :type "LinearColor Structure"))
  ;[1 1 1] Skin
  (bind _output_get (set `/Game/Blueprints/Customisation/SaveGame_Cosmetics.Skin Color` `Skin Color` (`self.Save`)))
  (`self.Server Set Skin Color` _output_get)
  (`self.Save Changes`))

(event `Server Set Skin Color`
  (params (Color :type "LinearColor Structure"))
  ;[1 1 1] Skin
  (set `self.Skin Color` Color))

(event `Server Set Color`
  (params (ID :type Integer) (`Color Palette` :type "/Game/Blueprints/Customisation/F_ArmorColor Structure"))
  ;[1 1 1] Colors
  (`KismetArrayLibrary.Array_Set` (`self.Replicated Armor Colors`) ID `Color Palette` true)
  (set `self.Replicated Armor Colors` (`self.Replicated Armor Colors`)))

(event `Server Set All Colors`
  (params (Color :type "/Game/Blueprints/Customisation/F_ArmorColor Structure"))
  ;[1 1 1] Colors
  (set `self.Replicated Armor Colors` (`|MakeArray` Color)))

(event `Client Set Cape ID`
  (params (`Cape ID` :type Byte))
  ;[1 1 1] Cape
  (bind _save (`self.Save`)
    (:`then`
      (bind _output_get (set `/Game/Blueprints/Customisation/SaveGame_Cosmetics.Cape ID` `Cape ID` _save))
      (`GameplayStatics.SaveGameToSlot` _save (`self.Slot Name`))
      (`self.Server Set Cape ID` _output_get))
    (:`else`)))

(event `Server Set Cape ID`
  (params (`Cape ID` :type Byte))
  ;[1 1 1] Cape
  (set `self.Cape ID` `Cape ID`))

(event `Preview Cape ID`
  (params (ID :type Integer))
  ;[1 1 1] Cape
  (`self.Set Cape` ID))

(event `Apply Replicated Cape`
  ;[1 1 1] Cape
  (`self.Set Cape` (`KismetMathLibrary.Conv_ByteToInt` (`self.Cape ID`))))

(fn `Apply Armor Params`
  (params (Color :type "/Game/Blueprints/Customisation/F_ArmorColor Structure") (Mesh :type "SkeletalMeshComponent Object Reference"))
  (bind (_color_primary _color_secondary _color_metal_primary _color_metal_secondary _color_metal_dark _color_leather_primary _color_leather_secondary) (break `/Game/Blueprints/Customisation/F_ArmorColor` (`local.Color`)))
  (`/Engine/EditorBlueprintResources/StandardMacros.IsValid` Mesh
    (:`Is Valid`
      (for (_array_element _array_index) (`|MakeArray` _color_primary _color_secondary _color_metal_primary _color_metal_secondary _color_metal_dark _color_leather_primary _color_leather_secondary)
        (`MeshComponent.SetVectorParameterValueOnMaterials` (`local.Mesh`) (`|GetArrayItem` (`|MakeArray` "Color_Primary" "Color_Secondary" "Color_Metal_Primary" "Color_Metal_Secondary" "Color_Metal_Dark" "Color_Leather_Primary" "Color_Leather_Secondary" :!type "Name") _array_index) (`KismetMathLibrary.Conv_LinearColorToVector` _array_element))))))

(fn `Apply Loaded Data`
  (bind _save (`self.Save`))
  (bind _armor_colors (`/Game/Blueprints/Customisation/SaveGame_Cosmetics.Armor Colors` _save))
  (for (_array_element _array_index) (`/Game/Blueprints/Customisation/SaveGame_Cosmetics.Armor Mesh` _save)
    (bind _skeletal_mesh_comp (`self.Set Skeletal Mesh` _array_element))
    (if (`KismetArrayLibrary.Array_IsValidIndex` _armor_colors _array_index)
      (`self.Apply Armor Params` (`|GetArrayItem` _armor_colors _array_index) _skeletal_mesh_comp)
      (else
        (`KismetArrayLibrary.Array_Set` (`/Game/Blueprints/Customisation/SaveGame_Cosmetics.Armor Colors` (`self.Save`)) _array_index (`self.Default Color`) true))))
  (`self.Client Set Cape ID` (`/Game/Blueprints/Customisation/SaveGame_Cosmetics.Cape ID` (`self.Save`))))

(fn `Apply Replicated Colors`
  (bind _replicated_armor_colors (`self.Replicated Armor Colors`))
  (bind _meshes (`self.Get Skeletal Meshes`))
  (for (_array_element _array_index) _meshes
    (`self.Apply Armor Params` (`|GetArrayItem` _replicated_armor_colors (`KismetMathLibrary.Min` _array_index (`KismetArrayLibrary.Array_LastIndex` _replicated_armor_colors))) _array_element)))

(fn `Apply Skin Color`
  (params (Comp :type "MeshComponent Object Reference") (`Preview Color` :type "Vector Structure") (Preview :type Boolean))
  (bind _returnvalue (select `bool` Preview :`false` (`KismetMathLibrary.Conv_LinearColorToVector` (`self.Skin Color`)) :`true` `Preview Color`))
  (`MeshComponent.SetVectorParameterValueOnMaterials` Comp "Color_Skin" _returnvalue)
  (`MeshComponent.SetVectorParameterValueOnMaterials` Comp "Color_Stubble" (* _returnvalue 0.7)))

(fn `Check Guard Armor Achievement`
  (locals (`L Guard Armor Count` :type Integer))
  (if (`self.Locally Owned`)
    (for _array_element (`self.Replicated Row Handles`)
      (bind (_datatable _rowname) (break `DataTableRowHandle` _array_element))
      (if (`KismetStringLibrary.Contains` (`KismetStringLibrary.Conv_NameToString` _rowname) "Guards")
        (switch `string` (`KismetStringLibrary.Conv_ObjectToString` _datatable)
          (:`DT_Helmets`
            _)
          (:`DT_Torso`
            _)
          (:`DT_Hips`
            _))
        (bind _result (`/Engine/EditorBlueprintResources/StandardMacros.IncrementInt` (`local.L Guard Armor Count`))
          (:`  `
            (if (>= _result 3)
              (`|SpawnActorFromClass` "/Game/_Guards/OnlineSubsystem/Achievements/BP_AchievementProgressor.BP_AchievementProgressor_C" (`KismetMathLibrary.Conv_VectorToTransform` (0.0 0.0 0.0)) "AlwaysSpawn" "MultiplyWithRoot" null "" "FullArmor" 0 null)
              (return))))))))

(fn `Get Skeletal Mesh From DataTable`
  (params (`Data Table` :type "DataTable Object Reference"))
  (returns (Mesh :type "SkeletalMeshComponent Object Reference") (Index :type Integer))
  (bind _keys (`BlueprintMapLibrary.Map_Keys` (`self.Skeletal Meshes`)))
  (for (_array_element _array_index) _keys
    (bind (_value _returnvalue) (`BlueprintMapLibrary.Map_Find` (`self.Skeletal Meshes`) _array_element))
    (if _returnvalue
      (if (== (`.DataTable` (break `DataTableRowHandle` _value)) (`local.Data Table`))
        (return _array_element _array_index))))
  (return null -1))

(fn `Get Skeletal Meshes`
  (returns (Meshes :type "Array of SkeletalMeshComponent Object Reference"))
  (bind _keys (`BlueprintMapLibrary.Map_Keys` (`self.Skeletal Meshes`)))
  (return _keys))

(fn `Load Save`
  (locals (`L new save` :type Boolean :default false))
  ;[1 1 1] Load save data, apply it locally, then send any outdated info to serrver
  (bind _returnvalue (`GameplayStatics.DoesSaveGameExist` (`self.Slot Name`)))
  (if _returnvalue
    (bind _returnvalue_2 (`GameplayStatics.LoadGameFromSlot` (`self.Slot Name`)))
    (bind _assave_game_cosmetics (cast `/Game/Blueprints/Customisation/SaveGame_Cosmetics` _returnvalue_2))
    (set `self.Save` _assave_game_cosmetics)
    (else
      (bind _returnvalue_3 (`GameplayStatics.CreateSaveGameObject` "/Game/Blueprints/Customisation/SaveGame_Cosmetics.SaveGame_Cosmetics_C"))
      (set `self.Save` _returnvalue_3)
      (set `local.L new save` true)))
  (`self.Apply Loaded Data`)
  (`self.Update All` (`local.L new save`)))

(fn `OnRep_Cape ID`
  (`self.Set Cape` (`KismetMathLibrary.Conv_ByteToInt` (`self.Cape ID`)))
  (`self.Data Updated`))

(fn `OnRep_Replicated Armor Colors`
  (`self.Apply Replicated Colors`)
  (`self.Data Updated`))

(fn `OnRep_Replicated Row Handles`
  (`self.Update Meshes`)
  (`self.Data Updated`)
  (`KismetSystemLibrary.K2_ClearAndInvalidateTimerHandle` (`self.Reload Fallback`)))

(fn `OnRep_Skin Color`
  (bind _keys (`BlueprintMapLibrary.Map_Keys` (`self.Skeletal Meshes`)))
  (for _array_element _keys
    (`self.Apply Skin Color` _array_element))
  (`self.Data Updated`))

(fn `Preview Armor Colors`
  (params (Color :type "/Game/Blueprints/Customisation/F_ArmorColor Structure") (ID :type Integer :default -1))
  ;[1 1 1] Color all pieces
  (bind _keys (`BlueprintMapLibrary.Map_Keys` (`self.Skeletal Meshes`)))
  (if (< ID 0)
    (for _array_element _keys
      (`self.Apply Armor Params` (`local.Color`) _array_element))
    (else
      ;[1 1 1] Color a single piece
      (if (`KismetArrayLibrary.Array_IsValidIndex` _keys ID)
        (`self.Apply Armor Params` (`local.Color`) (`|GetArrayItem` _keys ID))))))

(fn `Reset Materials`
  (params (`In Mesh` :type "SkeletalMeshComponent Object Reference"))
  (bind _replicated_armor_colors (`self.Replicated Armor Colors`))
  (for _index (range (`PrimitiveComponent.GetNumMaterials` `In Mesh`))
    (`PrimitiveComponent.SetMaterial` `In Mesh` _index null) ; reset
  )
  (bind _meshes (`self.Get Skeletal Meshes`))
  (bind _returnvalue (`KismetMathLibrary.Min` (`KismetArrayLibrary.Array_Find` _meshes (`local.In Mesh`)) (`KismetArrayLibrary.Array_LastIndex` _replicated_armor_colors)))
  (if (`KismetArrayLibrary.Array_IsValidIndex` _replicated_armor_colors _returnvalue)
    (`self.Apply Armor Params` (`|GetArrayItem` _replicated_armor_colors _returnvalue) (`local.In Mesh`))))

(fn `Save Changes`
  (bind _save (`self.Save`)
    (:`then`
      (bind _values (`BlueprintMapLibrary.Map_Values` (`self.Skeletal Meshes`)))
      (set `/Game/Blueprints/Customisation/SaveGame_Cosmetics.Armor Mesh` _values _save)
      (set `/Game/Blueprints/Customisation/SaveGame_Cosmetics.Skin Color` (`self.Skin Color`) _save)
      (`GameplayStatics.SaveGameToSlot` _save (`self.Slot Name`)))
    (:`else`)))

(fn `Set Armor Piece Color`
  (params (`Color Palette` :type "/Game/Blueprints/Customisation/F_ArmorColor Structure") (Index :type Integer))
  (`KismetArrayLibrary.Array_Set` (`/Game/Blueprints/Customisation/SaveGame_Cosmetics.Armor Colors` (`self.Save`)) Index `Color Palette` true)
  (`GameplayStatics.SaveGameToSlot` (`self.Save`) (`self.Slot Name`))
  (`self.Server Set Color` Index (`local.Color Palette`)))

(fn `Set Cape`
  (params (ID :type Integer))
  (`/Engine/EditorBlueprintResources/StandardMacros.Can Execute Cosmetic Events`
    (:`True`
      (bind _outrownames (`DataTableFunctionLibrary.GetDataTableRowNames` "/Game/Blueprints/Customisation/Capes/DT_Capes.DT_Capes"))
      (bind _returnvalue (`|GetDataTableRow` "/Game/Blueprints/Customisation/Capes/DT_Capes.DT_Capes" (`|GetArrayItem` _outrownames ID))
        (:`then`
          (bind _asbp_character_template_player (cast `/Game/Blueprints/Core/BP_Character_Template_Player` (`self.GetOwner`)))
          (`|ExecutionSequence`
            (:`then_0`
              (bind (_cape _mat) (break `/Game/Blueprints/Customisation/Capes/F_Cape` _returnvalue))
              (if (`KismetSystemLibrary.IsValidSoftObjectReference` _cape)
                (bind _returnvalue_2 (`KismetSystemLibrary.LoadAsset_Blocking` _cape))
                (bind _asskeletal_mesh (cast `SkeletalMesh` _returnvalue_2))
                (bind _cape_2 (`/Game/Blueprints/Core/BP_Character_Template_Player.Cape` _asbp_character_template_player))
                (`SkeletalMeshComponent.SetSkeletalMeshAsset` _cape_2 _asskeletal_mesh)
                (else
                  (`SkeletalMeshComponent.SetSkeletalMeshAsset` _cape_2 null))))
            (:`then_1`
              (bind _returnvalue_3 (`KismetSystemLibrary.LoadAsset_Blocking` _mat))
              (bind _asmaterial_interface (cast `MaterialInterface` _returnvalue_3))
              (`PrimitiveComponent.SetMaterial` _cape_2 0 _asmaterial_interface))
            (:`then_2`
              (`SceneComponent.SetVisibility` _cape_2 true false))))
        (:`RowNotFound`
          (return))))))

(fn `Set Color on All Armor`
  (params (`Color Palette` :type "/Game/Blueprints/Customisation/F_ArmorColor Structure"))
  (bind _meshes (`self.Get Skeletal Meshes`))
  (for (_ _array_index) _meshes
    (`self.Set Armor Piece Color` `Color Palette` _array_index)))

(fn `Set Mesh`
  (params (Row :type "DataTableRowHandle Structure"))
  (for (_array_element _array_index) (`self.Replicated Row Handles`)
    (if (== (`.DataTable` (break `DataTableRowHandle` _array_element)) (`.DataTable` (break `DataTableRowHandle` Row)))
      (`KismetArrayLibrary.Array_Set` (`self.Replicated Row Handles`) _array_index (`local.Row`) true)
      (set `self.Replicated Row Handles` (`self.Replicated Row Handles`))
      (return)))
  (`KismetArrayLibrary.Array_Add` (`self.Replicated Row Handles`) Row)
  (set `self.Replicated Row Handles` (`self.Replicated Row Handles`)))

(fn `Set No See Mesh Vis`
  (params (`Should See` :type Boolean))
  (bind _skeletal_meshes (`self.Skeletal Meshes`))
  (bind _keys (`BlueprintMapLibrary.Map_Keys` _skeletal_meshes))
  (for _array_element _keys
    (if (`KismetArrayLibrary.Array_Contains` (`self.Owner NoSee Meshes`) (`KismetStringLibrary.Conv_ObjectToString` (`.DataTable` (break `DataTableRowHandle` (`BlueprintMapLibrary.Map_Find` _skeletal_meshes _array_element)))))
      (`PrimitiveComponent.SetOwnerNoSee` _array_element (not (`local.Should See`))))))

(fn `Set Skeletal Mesh`
  (params (Row :type "DataTableRowHandle Structure"))
  (returns (`Skeletal Mesh Comp` :type "SkeletalMeshComponent Object Reference"))
  (locals (`L Skeletal Mesh Component` :type "SkeletalMeshComponent Object Reference") (`L New Mesh` :type "SkeletalMesh Object Reference") (`L Skel` :type "SkeletalMeshComponent Object Reference") (`L Data` :type "/Game/Blueprints/Customisation/F_CosmeticDefinition Structure") (`L New Data` :type Boolean :default false) (`L Row` :type "DataTableRowHandle Structure"))
  (bind _skeletal_meshes (`self.Skeletal Meshes`))
  (bind _l_skeletal_mesh_component (`local.L Skeletal Mesh Component`))
  (bind _l_skeletal_mesh_component_2 (`local.L Skeletal Mesh Component`))
  (bind _l_skeletal_mesh_component_3 (`local.L Skeletal Mesh Component`))
  (bind _l_skeletal_mesh_component_4 (`local.L Skeletal Mesh Component`))
  (bind _skeletal_meshes_2 (`self.Skeletal Meshes`))
  (bind _l_skeletal_mesh_component_5 (`local.L Skeletal Mesh Component`))
  (bind ((`Socket_18_6F15215C46B9034A0BA75DBEE98C4AB9` _socket) (`RelativeTransform_23_CDAA35D945D78B513A8BB9A1F9EC6AD9` _relativetransform)) (break `/Game/Blueprints/Customisation/F_CosmeticDefinition` (`local.L Data`)))
  (bind (_skelmesh _name _cost _socket_2 _relativetransform_2) (break `/Game/Blueprints/Customisation/F_CosmeticDefinition` (`local.L Data`)))
  (bind (_datatable _rowname) (break `DataTableRowHandle` (`local.L Row`)))
  (bind _ascharacter (cast `Character` (`self.GetOwner`) :!pure true))
  (bind _mesh (`Character.Mesh` (cast `Character` (`self.GetOwner`) :!pure true)))
  ;[1 1 1] Cache new mesh to apply
  (set `local.L Row` Row)
  (`/Engine/EditorBlueprintResources/StandardMacros.Can Execute Cosmetic Events`
    (:`True`
      (`/Engine/EditorBlueprintResources/StandardMacros.IsValid` _datatable
        (:`Is Valid`
          (bind _returnvalue (`|GetDataTableRow` _datatable _rowname)
            (:`then`
              (set `local.L Data` _returnvalue)
              (bind _skelmesh_2 (break `/Game/Blueprints/Customisation/F_CosmeticDefinition` _returnvalue))
              (if (`KismetSystemLibrary.IsValidSoftObjectReference` _skelmesh_2)
                (bind _returnvalue_2 (`KismetSystemLibrary.LoadAsset_Blocking` _skelmesh_2))
                (bind _asskeletal_mesh (cast `SkeletalMesh` _returnvalue_2))
                (set `local.L New Mesh` _asskeletal_mesh)
                (else
                  (set `local.L New Mesh` null :!label _label))))
            (:`RowNotFound`
              (bind _outrownames (`DataTableFunctionLibrary.GetDataTableRowNames` _datatable))
              (bind _output (`|GetArrayItem` _outrownames))
              (set `local.L Row` (make `DataTableRowHandle` _datatable _output))
              (bind _returnvalue_3 (`|GetDataTableRow` _datatable _output)
                (:`then`
                  (bind _skelmesh_3 (break `/Game/Blueprints/Customisation/F_CosmeticDefinition` _returnvalue_3))
                  (if (`KismetSystemLibrary.IsValidSoftObjectReference` _skelmesh_3)
                    (bind _returnvalue_4 (`KismetSystemLibrary.LoadAsset_Blocking` _skelmesh_3))
                    (bind _asskeletal_mesh_2 (cast `SkeletalMesh` _returnvalue_4))
                    (set `local.L New Mesh` _asskeletal_mesh_2)
                    (else
                      (goto _label)))))))
          ;[1 1 1] Find existing mesh for this data table and update it
          (bind _values (`BlueprintMapLibrary.Map_Values` _skeletal_meshes))
          (for (_array_element _array_index) _values
            (if (== (`.DataTable` (break `DataTableRowHandle` _array_element)) (`.DataTable` (break `DataTableRowHandle` (`local.Row`))))
              (bind _keys (`BlueprintMapLibrary.Map_Keys` _skeletal_meshes))
              (set `local.L Skeletal Mesh Component` (`|GetArrayItem` _keys _array_index))
              (`SkinnedMeshComponent.SetSkinnedAssetAndUpdate` _l_skeletal_mesh_component_2 (`local.L New Mesh`) true)
              (`self.Reset Materials` _l_skeletal_mesh_component_2)
              (`BlueprintMapLibrary.Map_Remove` _skeletal_meshes_2 _l_skeletal_mesh_component_2)
              (`BlueprintMapLibrary.Map_Add` _skeletal_meshes_2 _l_skeletal_mesh_component_2 (`local.L Row`))
              (`self.Apply Skin Color` (`local.L Skeletal Mesh Component`))
              (`SceneComponent.K2_AttachToComponent` _l_skeletal_mesh_component_5 _mesh _socket "SnapToTarget" "SnapToTarget" "SnapToTarget" true)
              (`SceneComponent.K2_SetRelativeTransform` _l_skeletal_mesh_component_5 _relativetransform false false)
              (if (== _socket "None")
                (`SkinnedMeshComponent.SetLeaderPoseComponent` (`local.L Skeletal Mesh Component`) _mesh false false))
              (return (`local.L Skeletal Mesh Component`))))
          ;[1 1 1] Cannot find mapped skeletalmesh& data table combo - create new skeletal mesh
          (bind _returnvalue_5 (`|AddComponentByClass` :`self` (`self.GetOwner`) :`Class` "/Script/Engine.SkeletalMeshComponent"))
          (`BlueprintMapLibrary.Map_Add` (`self.Skeletal Meshes`) _returnvalue_5 (`local.L Row`))
          (set `SceneComponent.bUseAttachParentBound` true _returnvalue_5)
          (set `local.L Skeletal Mesh Component` _returnvalue_5)
          (`SkinnedMeshComponent.SetSkinnedAssetAndUpdate` _l_skeletal_mesh_component (`local.L New Mesh`) true)
          (`self.Reset Materials` _l_skeletal_mesh_component)
          (`SceneComponent.K2_AttachToComponent` (`local.L Skeletal Mesh Component`) (`Character.Mesh` _ascharacter) _socket_2 "SnapToTarget" "SnapToTarget" "SnapToTarget" true)
          (`SceneComponent.K2_SetRelativeTransform` (`local.L Skeletal Mesh Component`) _relativetransform_2 false false)
          (if (== _socket_2 "None")
            (`SkinnedMeshComponent.SetLeaderPoseComponent` _l_skeletal_mesh_component_4 (`Character.Mesh` _ascharacter) false false))
          (`PrimitiveComponent.SetCastHiddenShadow` _l_skeletal_mesh_component_4 true)
          (`PrimitiveComponent.SetCollisionEnabled` _l_skeletal_mesh_component_4 "NoCollision")
          (`self.SetComponentTickEnabled` (`local.L Skeletal Mesh Component`) false)
          (`|ExecutionSequence`
            (:`then_0`
              ;[1 1 1] Show and hide for owner
              (`self.Save`
                (:`then`
                  (`PrimitiveComponent.SetOnlyOwnerSee` _l_skeletal_mesh_component_3 (`KismetArrayLibrary.Array_Contains` (`self.Owner OnlySee Meshes`) (`KismetSystemLibrary.GetDisplayName` (`.DataTable` (break `DataTableRowHandle` (`local.Row`))))))
                  (`PrimitiveComponent.SetOwnerNoSee` _l_skeletal_mesh_component_3 (`KismetArrayLibrary.Array_Contains` (`self.Owner NoSee Meshes`) (`KismetSystemLibrary.GetDisplayName` (`.DataTable` (break `DataTableRowHandle` (`local.Row`)))))))
                (:`else`)))
            (:`then_1`
              ;[1 1 1] Apply Dynamic Material
              (`self.Apply Skin Color` (`local.L Skeletal Mesh Component`)))
            (:`then_2`
              ;[1 1 1] return mesh
              (return (`local.L Skeletal Mesh Component`)))))))))

(fn `Set Stencil`
  (params (Enabled :type Boolean) (ID :type Integer))
  (bind _keys (`BlueprintMapLibrary.Map_Keys` (`self.Skeletal Meshes`)))
  (for _array_element _keys
    (`PrimitiveComponent.SetRenderCustomDepth` _array_element Enabled)
    (`PrimitiveComponent.SetCustomDepthStencilValue` _array_element ID)))

(fn `Update All`
  (params (Save :type Boolean :default true))
  (locals (`L Values` :type "Map of SkeletalMeshComponent Object Reference to DataTableRowHandle Structure"))
  ;[1 1 1] Owner send any edited skeletal mesh settings to server to replicate
  (set `local.L Values` (`self.Skeletal Meshes`))
  (`BlueprintMapLibrary.Map_Values` (`local.L Values`))
  (`self.Server Set All Meshes` (`/Game/Blueprints/Customisation/SaveGame_Cosmetics.Armor Mesh` (`self.Save`)))
  (`|ExecutionSequence`
    (:`then_0`
      ;[1 1 1] Colors
      (`self.Server Set Skin Color` (`/Game/Blueprints/Customisation/SaveGame_Cosmetics.Skin Color` (`self.Save`)))
      (for (_array_element _array_index) (`/Game/Blueprints/Customisation/SaveGame_Cosmetics.Armor Colors` (`self.Save`))
        (`self.Server Set Color` _array_index _array_element)))
    (:`then_1`
      ;[1 1 1] Save
      (if (`local.Save`)
        (bind _save (`self.Save`)
          (:`then`
            (bind _values (`BlueprintMapLibrary.Map_Values` (`self.Skeletal Meshes`)))
            (set `/Game/Blueprints/Customisation/SaveGame_Cosmetics.Armor Mesh` _values _save)
            (set `/Game/Blueprints/Customisation/SaveGame_Cosmetics.Skin Color` (`self.Skin Color`) _save)
            (`GameplayStatics.SaveGameToSlot` _save (`self.Slot Name`)))
          (:`else`))))))

(fn `Update Meshes`
  (for _array_element (`self.Replicated Row Handles`)
    (`self.Set Skeletal Mesh` _array_element))
  (`self.Check Guard Armor Achievement`))