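; Loot spawner component that rolls a chance and count, then launches loot beams from a given location to scattered ground points.
; Settings optionally come from DT_Loot, matched on owner class.
; SpawnLoot validates random points with traces and predicted projectile arcs, with an attempt cap, passing velocities to Niagara beams.
; Niagara's particle callback returns positions where the authority spawns probability-weighted physics items, while sounds play only where cosmetic events run.
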(event `MC Create Beam`
  (params (Yaw :type "Float (single-precision)") (Velocity :type "Vector Structure") (Location :type "Vector Structure"))
  ;[1 1 1] Spawnable
  (bind _returnvalue (`NiagaraFunctionLibrary.SpawnSystemAtLocation` (`self.Particle Beam`) Location (`KismetMathLibrary.MakeRotator` 0.0 0.0 Yaw)))
  (`/Engine/EditorBlueprintResources/StandardMacros.IsValid` _returnvalue
    (:`Is Valid`
      (`NiagaraComponent.SetVariableVec3` _returnvalue "User.CustomVelocity" Velocity)
      (`NiagaraComponent.SetVariableObject` _returnvalue "User.BlueprintCallback" self)
      (`/Engine/EditorBlueprintResources/StandardMacros.Can Execute Cosmetic Events`
        (:`True`
          (bind _loot_beam_sound (`self.Loot Beam Sound`)
            (:`then`
              (`GameplayStatics.PlaySoundAtLocation` _loot_beam_sound Location (struct) 1.0 1.0 0.0 "/Game/Blueprints/GAS/Cues/Sounds/ATT_Close.ATT_Close" null null null))
            (:`else`)))))))

(event `self.ReceiveParticleData`
  (params (Data :type "Array of BasicParticleData Structure (by ref)") (NiagaraSystem :type "NiagaraSystem Object Reference") (SimulationPositionOffset :type "Vector Structure (by ref)"))
  ;[1 1 1] Spawnable
  (for _array_element Data
    (`|ExecutionSequence`
      (:`then_0`
        (`/Engine/EditorBlueprintResources/ActorComponentMacros.Switch Has Authority`
          (:`Authority`
            (bind _outitem (`self.Get Random Loot`))
            (if (`KismetSystemLibrary.IsValidSoftClassReference` _outitem)
              (bind _returnvalue (`KismetSystemLibrary.LoadClassAsset_Blocking` _outitem))
              (bind _asbp_item (castclass `/Game/Blueprints/Items/BP_Item` _returnvalue))
              (bind _position (break `BasicParticleData` _array_element))
              (bind _returnvalue_2 (`|SpawnActorFromClass` _asbp_item (`KismetMathLibrary.MakeTransform` (+ _position (0.0 0.0 50.0)) (`KismetMathLibrary.RandomRotator` true)) "AlwaysSpawn" "SelectDefaultAtRuntime" null null))
              (set `/Game/Blueprints/Items/BP_Item.Physics Enabled` true _returnvalue_2)
              (`/Game/Blueprints/Items/BP_Item.Set White Fill` _returnvalue_2 true)))))
      (:`then_1`
        (`/Engine/EditorBlueprintResources/StandardMacros.Can Execute Cosmetic Events`
          (:`True`
            (bind _loot_spawned_sound (`self.Loot Spawned Sound`)
              (:`then`
                (`GameplayStatics.PlaySoundAtLocation` _loot_spawned_sound _position (struct) 1.0 1.0 0.0 "/Game/Blueprints/GAS/Cues/Sounds/ATT_Close.ATT_Close" null null null))
              (:`else`))))))))

(fn `Get Random Loot`
  (returns (OutItem :type "/Game/Blueprints/Items/BP_Item Soft Class Reference"))
  (locals (Items :type "Array of /Game/Blueprints/Items/BP_Item Soft Class Reference"))
  (for _array_element (`.Loot_25_F15E589C4573B0E11DF665BEF6558223` (break `/Game/Blueprints/LootSpawner/F_LootConfig` (`self.Loot Config`)))
    (bind (_item _probability) (break `/Game/Blueprints/LootSpawner/F_LootSpawnable` _array_element))
    (for _ (range (+ (`KismetMathLibrary.Max` (- _probability 1)) 1))
      (`KismetArrayLibrary.Array_Add` (`local.Items`) _item)))
  (return (`KismetArrayLibrary.Array_Random` (`local.Items`))))

(fn `Load Data`
  (returns (Valid :type Boolean))
  (if (`self.Use DT_Loot`)
    (bind _outrownames (`DataTableFunctionLibrary.GetDataTableRowNames` "/Game/Blueprints/LootSpawner/DT_Loot.DT_Loot"))
    (for _array_element _outrownames
      (bind _returnvalue (`|GetDataTableRow` "/Game/Blueprints/LootSpawner/DT_Loot.DT_Loot" _array_element)
        (:`then`
          (if (== (`.FractureClass_2_F73AF20443C0FAB31C0A1484BD78C8B1` (break `/Game/Blueprints/LootSpawner/F_LootConfig` _returnvalue)) (`|ConvertAsset` (`GameplayStatics.GetObjectClass` (`self.GetOwner`))))
            (set `self.Loot Config` _returnvalue)
            (return true)))))
    (return false)
    (else
      (return true))))

(fn `Spawn Loot`
  (params (`In Location` :type "Vector Structure"))
  (locals (`L Count` :type Integer) (`L Rand Point` :type "Vector Structure" :default (0.0 0.0 0.0)) (`L Custom Velocity` :type "Vector Structure" :default (200.0 0.0 500.0)) (Attempts :type Integer) (`L Location` :type "Vector Structure" :default (0.0 0.0 0.0)))
  (bind _in_location (`local.In Location`))
  (bind ((`ChancetoCreateLoot_5_2FFD82414AC65B4B0DA7E2B2C090F56E` _chancetocreateloot) (`CountMin_11_A088869D4B4322E5A4566AA0461414E8` _countmin) (`CountMax_12_EAD9EE7C472B22BDC2B904900AC686D7` _countmax)) (break `/Game/Blueprints/LootSpawner/F_LootConfig` (`self.Loot Config`)))
  (bind (_returnvalue_roll _returnvalue_pitch _returnvalue_yaw) (`KismetMathLibrary.BreakRotator` (`KismetMathLibrary.FindLookAtRotation` _in_location (`local.L Location`))))
  (bind (_x _y) (`KismetMathLibrary.BreakVector2D` (`.SpawnXYRange_16_3A34E4454B778463AB22DAB69F4526F5` (break `/Game/Blueprints/LootSpawner/F_LootConfig` (`self.Loot Config`)))))
  (bind _valid (`self.Load Data`))
  (if _valid
    (if (`KismetMathLibrary.RandomBoolWithWeight` _chancetocreateloot)
      (set `local.L Count` (`KismetMathLibrary.RandomIntegerInRange` _countmin _countmax))
      (while (> (`local.L Count`) 0)
        (`/Engine/EditorBlueprintResources/StandardMacros.IncrementInt` (`local.Attempts`)
          (:`  `
            (`|ExecutionSequence`
              (:`then_0`
                (set `local.L Rand Point` (`KismetMathLibrary.RandomPointInBoundingBox` (`local.In Location`) (/ (`KismetMathLibrary.MakeVector` _x _y 1.0) 2.0)))
                (bind _outhits (`KismetSystemLibrary.LineTraceMulti` (`local.L Rand Point`) (- (`local.L Rand Point`) (0.0 0.0 500.0)) "TraceTypeQuery2" false (`|MakeArray` (`self.GetOwner`)) (`self.Debug`)))
                (for _array_element _outhits
                  (set `local.L Location` (`.Location` (`GameplayStatics.BreakHitResult` _array_element)))
                  (bind (_outhit _returnvalue) (`KismetSystemLibrary.LineTraceSingle` (`local.In Location`) (+ (`local.L Location`) (0.0 0.0 5.0)) "TraceTypeQuery2" false (`|MakeArray` (`self.GetOwner`)) (`self.Debug`))) ; is there an obstacle between the center of this asset and the end location
                  (if (not _returnvalue)
                    (bind _outlaunchvelocity (`GameplayStatics.SuggestProjectileVelocity_CustomArc` (`local.In Location`) (`local.L Location`) 0.0 (`KismetMathLibrary.RandomFloatInRange` 0.1 0.3)))
                    (set `local.L Custom Velocity` _outlaunchvelocity)
                    (bind (_outhit_2 _outpathpositions _outlasttracedestination _returnvalue_2) (`GameplayStatics.Blueprint_PredictProjectilePath_ByTraceChannel` (`local.In Location`) (`local.L Custom Velocity`) true 2.0 "ECC_Camera" false (`|MakeArray` (`self.GetOwner`)) (`self.Debug`) 2.0 15.0 5.0))
                    (if _returnvalue_2
                      (`self.MC Create Beam` _returnvalue_yaw (`local.L Custom Velocity`) _in_location)
                      (`/Engine/EditorBlueprintResources/StandardMacros.DecrementInt` (`local.L Count`))))))
              (:`then_1`
                (if (> (`local.Attempts`) 50)
                  (`/Engine/EditorBlueprintResources/StandardMacros.DecrementInt` (`local.L Count`)
                    (:`  `
                      (set `local.Attempts` 0)
                      (`KismetSystemLibrary.PrintString` "reached 50 attempts in Loot Component"))))))))))))