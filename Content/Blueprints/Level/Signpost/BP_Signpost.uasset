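; Level signpost actor that displays an image for the selected crisis mission.
; Once a crisis component is selected or loads data, it looks up the mission's texture in a per-district map, falling back to the perp's face for arrest missions, else hides and disables collision.
; Textures load synchronously into a dynamic material, only where cosmetic events can execute.
; The arrow is hidden for all but three mission types; its bob timeline is never triggered.
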(event `self.ReceiveBeginPlay`
  (bind _selected (`/Game/Blueprints/Crisis/BPFL_Crisis.Bind to Crisis Selected` (delegate `On Crisis Selected`)))
  (`/Engine/EditorBlueprintResources/StandardMacros.IsValid` _selected
    (:`Is Valid`
      (`self.On Crisis Selected` _selected))))

(event `On Crisis Selected`
  (params (Comp :type "/Game/Blueprints/Crisis/BP_Crisis_Component Object Reference"))
  (bind _crisis_comp (`self.Crisis Comp`))
  (bind (_intel _doom _mission _daysleft _arrestperp) (break `/Game/Blueprints/Crisis/F_CrisisMission` (`/Game/Blueprints/Crisis/BP_Crisis_Component.Get Selected Mission` (`self.Crisis Comp`))))
  (bind (_datatable _rowname) (break `DataTableRowHandle` _arrestperp))
  (bind (_value _returnvalue) (`BlueprintMapLibrary.Map_Find` (select `byte` (`/Game/Blueprints/Crisis/BP_Crisis_Component.District ID` _crisis_comp) :`0` (`self.D1 Texture`) :`1` (`self.D2 Texture`) :`2` (`self.D3 Texture`)) _mission))
  (set `self.Crisis Comp` Comp)
  (add `/Game/Blueprints/Crisis/BP_Crisis_Component.Data Loaded` (`self.Crisis Comp`) (delegate `Data Loaded_Event`))
  (if (`/Game/Blueprints/Crisis/BP_Crisis_Component.District Selected` _crisis_comp) :!label _label
    (`|ExecutionSequence`
      (:`then_0`
        (if _returnvalue
          (`self.Set Texture` _value)
          (`SceneComponent.SetVisibility` (`self.StaticMeshComponent`) true true)
          (`self.SetActorEnableCollision` true)
          (elif (`|EnumEquality` _mission "NewEnumerator11")
            (bind _returnvalue_2 (`|GetDataTableRow` _datatable _rowname)
              (:`then`
                (`self.Set Texture` (`.Face_61_2B2F1F344C0503ABB20198964E4FC096` (break `/Game/Blueprints/Core/PolygonAI/Config/F_Character_Setup` _returnvalue_2)))
                (`SceneComponent.SetVisibility` (`self.StaticMeshComponent`) true true)
                (`self.SetActorEnableCollision` true)))
            (else
              (`SceneComponent.SetVisibility` (`self.StaticMeshComponent`) false true)
              (`self.SetActorEnableCollision` false)))))
      (:`then_1`
        (if (not (`self.Show Arrow` _mission))
          (`SceneComponent.SetVisibility` (`self.Arrow`) false true))))))

(event `Data Loaded_Event`
  (params (`Crisis Comp` :type "/Game/Blueprints/Crisis/BP_Crisis_Component Object Reference"))
  (set `self.Crisis Comp` `Crisis Comp`)
  (goto _label))

(fn `OnRep_Texture`)

(fn `Set Texture`
  (params (Texture :type "Texture2D Soft Object Reference"))
  (`/Engine/EditorBlueprintResources/StandardMacros.Can Execute Cosmetic Events`
    (:`True`
      (bind _returnvalue (`PrimitiveComponent.CreateDynamicMaterialInstance` (`self.Plane`) 0 "/Game/Blueprints/Level/Signpost/M_Signpost.M_Signpost" "None"))
      (bind _returnvalue_2 (`KismetSystemLibrary.LoadAsset_Blocking` Texture))
      (bind _astexture_2d (cast `Texture2D` _returnvalue_2))
      (`MaterialInstanceDynamic.SetTextureParameterValue` _returnvalue "Texture" _astexture_2d))))

(fn `Show Arrow`
  (params (InputPin :type "/Game/_Guards/UserInterface/WorldMap/E_MissionType Enum" :default "NewEnumerator0"))
  (returns (ReturnValue :type Boolean))
  (return (or (`|EnumEquality` InputPin "NewEnumerator3") (`|EnumEquality` InputPin "NewEnumerator8") (`|EnumEquality` InputPin "NewEnumerator11"))))

(fn `UserConstructionScript`)