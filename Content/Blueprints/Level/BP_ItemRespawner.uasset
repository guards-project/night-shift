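; Level actor that replenishes BP_Item pickups placed inside its bounds when they are equipped or destroyed.
; On BeginPlay, the server finds items within that box and binds to their equip and EndPlay events.
; Either event spawns a same-class copy at the item's current transform.
; Each copy is rebound only to the kind of event that spawned it.
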(event `self.ReceiveBeginPlay`
  (bind (_origin _boxextent) (`self.GetActorBounds` false))
  (`/Engine/EditorBlueprintResources/ActorMacros.Switch Has Authority`
    (:`Authority`
      (bind _outactors (`GameplayStatics.GetAllActorsOfClass` "/Game/Blueprints/Items/BP_Item.BP_Item_C"))
      (for _array_element _outactors
        (if (`GeometryScriptLibrary_BoxFunctions.TestPointInsideBox` (`GeometryScriptLibrary_BoxFunctions.MakeBoxFromCenterSize` _origin (* _boxextent 2.0)) (`self.K2_GetActorLocation` _array_element))
          (add `/Game/Blueprints/Items/BP_Item.ItemEquip` _array_element (delegate `OnItemEquipped`))
          (add `self.OnEndPlay` _array_element (delegate `OnItemEndPlay`)))))))

(event `OnItemEquipped`
  (params (Item :type "/Game/Blueprints/Items/BP_Item Object Reference"))
  (remove `/Game/Blueprints/Items/BP_Item.ItemEquip` Item (delegate `OnItemEquipped`))
  (remove `self.OnEndPlay` Item (`|CreateDelegate` :!event `OnItemEndPlay`))
  (bind _returnvalue (`|SpawnActorFromClass` (`GameplayStatics.GetObjectClass` Item) (`self.GetTransform` Item) "Undefined" "SelectDefaultAtRuntime" null false null))
  (add `/Game/Blueprints/Items/BP_Item.ItemEquip` _returnvalue (`|CreateDelegate` :!event `OnItemEquipped`)))

(event `OnItemEndPlay` :!signature `self.OnEndPlay`
  (params (Actor :type "Actor Object Reference") (EndPlayReason :type "EEndPlayReason Enum" :default "Destroyed"))
  (switch `EEndPlayReason` EndPlayReason
    (:`Destroyed`
      (bind _returnvalue (`|SpawnActorFromClass` (`GameplayStatics.GetObjectClass` Actor) (`self.GetTransform` Actor) "Undefined" "SelectDefaultAtRuntime" null null))
      (add `self.OnEndPlay` _returnvalue (`|CreateDelegate` :!event `OnItemEndPlay`)))))

(fn `UserConstructionScript`)