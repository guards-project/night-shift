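; Interactable seat decoration that a character can sit on, leaving by interacting again or on taking damage.
; The server sets or clears Occupant, and its OnRep does the seating and unseating.
; Seating locks movement, disables capsule collision, snaps the character to SnapLocation and chains random sitting montages.
; The authority applies GE_Sitting and removes it by the Status.Sitting tag, which also blocks interaction with empty seats.
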(event `/Game/Primer/Primer_Interaction/BPI_Interact.Execute Interact`
  (params (User :type "Controller Object Reference"))
  ;[1 1 1] On interact server set occupant
  (`/Engine/EditorBlueprintResources/StandardMacros.IsValid` User
    (:`Is Valid`
      (`/Engine/EditorBlueprintResources/ActorMacros.Switch Has Authority`
        (:`Authority`
          (`self.Occupant`
            (:`then`
              (`self.Server Exit Seat`))
            (:`else`
              (bind _asbp_character_template (cast `/Game/Blueprints/Core/BP_Character_Template` (`Controller.K2_GetPawn` User)))
              (set `self.Occupant` _asbp_character_template))))))))

(event `Server Exit Seat`
  ;[1 1 1] On interact server set occupant
  (bind _occupant (`self.Occupant`)
    (:`then`
      (`/Game/Blueprints/Core/BP_Character_Template.Auth Set Can Move` _occupant true)
      (`/Game/Blueprints/Core/BP_Character_Template.Auth Set Seated` _occupant false)
      (set `self.Occupant` null))
    (:`else`)))

(event `Play Random Montage`
  ;[1 1 1] Random montage, once complete, play another
  ; If interrupted, i.e. BEANS, wait, and play another
  (bind _occupant (`self.Occupant`)
    (:`then`
      (`|PlayMontage` (`Character.Mesh` _occupant) (`KismetArrayLibrary.Array_Random` (`self.Sitting Montages`))
        (:`OnCompleted`
          (`self.Play Random Montage` :!label _label))
        (:`OnBlendOut`
          (goto _label))
        (:`OnInterrupted`
          (`KismetSystemLibrary.Delay` 2.0)
          (`self.Play Random Montage`))))
    (:`else`)))

(fn `Auth Update GE Sitting`
  (`/Engine/EditorBlueprintResources/ActorMacros.Switch Has Authority`
    (:`Authority`
      (bind _occupant (`self.Occupant`)
        (:`then`
          (`AbilitySystemComponent.BP_ApplyGameplayEffectToSelf` :`self` (`/Game/Blueprints/Core/BP_Character_Template.GSCAbilitySystem` _occupant) :`GameplayEffectClass` "/Game/Polygon/Animations/PolygonAnims/Sitting/GE_Sitting.GE_Sitting_C"))
        (:`else`
          (bind _last_occupant (`self.Last Occupant`)
            (:`then`
              (bind _returnvalue (`AbilitySystemComponent.RemoveActiveEffectsWithGrantedTags` (`/Game/Blueprints/Core/BP_Character_Template.GSCAbilitySystem` _last_occupant) (struct :`GameplayTags` (struct :`(TagName` "Status.Sitting")))))
              (`KismetSystemLibrary.PrintString` (`KismetStringLibrary.Conv_IntToString` _returnvalue)))
            (:`else`)))))))

(fn `Get Can Interact`
  (returns (ReturnValue :type Boolean))
  (bind _occupant (`self.Occupant`)
    (:`then`
      (return (`Pawn.IsLocallyControlled` _occupant)))
    (:`else`
      (return (not (`GSCBlueprintFunctionLibrary.HasMatchingGameplayTag` (`GameplayStatics.GetPlayerPawn` 0) (struct :`TagName` "Status.Sitting")))))))

(fn `Get Interact Text`
  (returns (Text :type Text))
  (bind _occupant (`self.Occupant`)
    (:`then`
      (return (select `bool` (`Pawn.IsLocallyControlled` _occupant) :`false` (`self.Occupied Text`) :`true` (`self.Exit Text`))))
    (:`else`
      (return (`self.Enter Text`)))))

(fn `On Occupant Health Changed`
  (params (Component :type "/Game/Blueprints/Core/Components/BP_Health_Component Object Reference") (Delta :type "Float (double-precision)") (`New Health` :type "Float (double-precision)") (`Damage Type` :type "DamageType Object Reference"))
  (if (< Delta 0.0)
    (`self.Server Exit Seat`)))

(fn `OnRep_Occupant`
  (bind (_returnvalue_roll _returnvalue_pitch _returnvalue_yaw) (`KismetMathLibrary.BreakRotator` (`self.K2_GetActorRotation`)))
  (bind (_returnvalue_roll_2 _returnvalue_pitch_2 _returnvalue_yaw_2) (`KismetMathLibrary.BreakRotator` (`self.K2_GetActorRotation`)))
  ;[1 1 1] On rep occupant play animations and lock movement
  (bind _occupant (`self.Occupant`)
    (:`then`
      (set `self.Last Occupant` _occupant)
      (`self.Play Random Montage`)
      (`/Game/Blueprints/Core/BP_Character_Template.Auth Set Can Move` _occupant false) ; stop movement
      (`/Game/Blueprints/Core/BP_Character_Template.Auth Set Seated` _occupant true) ; stop rotation
      (`PrimitiveComponent.SetCollisionEnabled` (`Character.CapsuleComponent` (`self.Occupant`)) "NoCollision") ; stops native capsule character logic \nmoving the actor location in next node
      (`self.K2_SetActorLocation` (`self.Occupant`) (+ (`KismetMathLibrary.TransformLocation` (`self.GetTransform`) (`self.Snap Location`)) (0.0 0.0 90.0)) false false) ; set location
      (`self.K2_SetActorRotation` (`self.Occupant`) (`KismetMathLibrary.MakeRotator` 0.0 0.0 _returnvalue_yaw) false) ; set rotation
      (`self.Auth Update GE Sitting`) ; deny GAS
      ;[1 1 1] Sitting local owner set control rotations
      (`/Engine/EditorBlueprintResources/StandardMacros.IsValid` (`Pawn.GetController` (`self.Occupant`))
        (:`Is Valid`
          (`Controller.SetControlRotation` (`Pawn.GetController` (`self.Occupant`)) (`KismetMathLibrary.MakeRotator` 0.0 0.0 _returnvalue_yaw_2)) ; local user camera rotation
          (bind _asbp_character_template_player (cast `/Game/Blueprints/Core/BP_Character_Template_Player` (`self.Occupant`)))
          (`/Game/Blueprints/Core/BP_Character_Template_Player.Refresh Rotation Setting` _asbp_character_template_player) ; refresh the settings for orientation and yaw usage
          (bind _occupant_2 (`self.Occupant`)
            (:`then`
              (add `/Game/Blueprints/Core/Components/BP_Health_Component.Health Changed` (`/Game/Blueprints/Core/BP_Character_Template.BP_Health_Component` _occupant_2) (`|CreateDelegate` :!event `On Occupant Health Changed`)))
            (:`else`)))))
    (:`else`
      ;[1 1 1] Unseat
      (bind _last_occupant (`self.Last Occupant`)
        (:`then`
          (`self.Auth Update GE Sitting`) ; allow GAS
          (`Character.StopAnimMontage` _last_occupant (`Character.GetCurrentMontage` _last_occupant)) ; stop the seated montage
          (`self.K2_AddActorLocalOffset` (`self.Last Occupant`) (50.0 0.0 0.0) false false) ; move the actor off the seat
          (`PrimitiveComponent.SetCollisionEnabled` (`Character.CapsuleComponent` (`self.Last Occupant`)) "QueryAndPhysics") ; re-enable the capsule collision that we disabled on seated
          (`/Engine/EditorBlueprintResources/StandardMacros.IsValid` (`Pawn.GetController` (`self.Last Occupant`))
            (:`Is Valid`
              (bind _asbp_character_template_player_2 (cast `/Game/Blueprints/Core/BP_Character_Template_Player` (`self.Last Occupant`)))
              (`/Game/Blueprints/Core/BP_Character_Template_Player.Refresh Rotation Setting` _asbp_character_template_player_2) ; refresh orientation and yaw movement settings
              (remove `/Game/Blueprints/Core/Components/BP_Health_Component.Health Changed` (`/Game/Blueprints/Core/BP_Character_Template.BP_Health_Component` (`self.Last Occupant`)) (`|CreateDelegate` :!event `On Occupant Health Changed`)))))
        (:`else`)))))

(fn `UserConstructionScript`
  (`parent.UserConstructionScript`)
  (`SceneComponent.K2_SetRelativeLocation` (`self.Visualizer`) (`self.Snap Location`) false false))