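; Street lamp decoration Blueprint that changes its appearance when its Light_DayNight_Toggle signals on or off.
; The turn-off event swaps the Lamp's first material slot to an unlit "Off" material.
; The turn-on event sets that slot with no material specified, which clears the override back to the mesh default.
; Construction only calls the parent script, and the default event nodes are disabled.
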(event `self.Light_Day-Night_Toggle.Light Turn On`
  (`PrimitiveComponent.SetMaterial` (`self.Lamp`) 0 null))

(event `self.Light_Day-Night_Toggle.Light Turn Off`
  (`PrimitiveComponent.SetMaterial` (`self.Lamp`) 0 "/Game/PolygonDarkFantasy/Materials/Alts/M_PolygonDarkFantasy_01_Off.M_PolygonDarkFantasy_01_Off"))

(fn `UserConstructionScript`
  (`parent.UserConstructionScript`))