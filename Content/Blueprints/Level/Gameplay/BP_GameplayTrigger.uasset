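; Level gameplay trigger that, on server-side overlap by an allowed class, sends activate messages to target actors and can stream in a level.
; Targets come from a preset list plus optional class-and-tag lookup, randomly capped by MaxCount, and are messaged one by one with a short delay.
; Overlap can also start a random number of timed re-triggers.
; Collision can switch off once or temporarily, and the actor destroys itself after its disable limit.
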(event `self.ReceiveActorBeginOverlap`
  (params (OtherActor :type "Actor Object Reference"))
  (`self.Handle Overlap` OtherActor))

(event `Trigger`
  (if (`self.Server Only`)
    (`/Engine/EditorBlueprintResources/ActorMacros.Switch Has Authority`
      (:`Authority`
        _)))
  (`self.Init Stagger Targets`)
  (`self.Stagger Activate`)
  (`|ExecutionSequence`
    (:`then_0`
      (`/Engine/EditorBlueprintResources/ActorMacros.Switch Has Authority`
        (:`Authority`
          (`self.Load Level`))))
    (:`then_1`
      (if (`self.Do Once`)
        (`PrimitiveComponent.SetCollisionEnabled` (`self.CollisionComponent`) "NoCollision")))))

(event `Load Level`
  (`/Engine/EditorBlueprintResources/StandardMacros.DoOnce` false
    (:`Completed`
      (if (not (`KismetStringLibrary.IsEmpty` (`self.Level to Load`)))
        (`GameplayStatics.LoadStreamLevel` (`KismetStringLibrary.Conv_StringToName` (`self.Level to Load`)) true)))))

(event `Stagger Activate`
  (bind _stagger_targets (`self.Stagger Targets`))
  (if (`KismetArrayLibrary.Array_IsValidIndex` _stagger_targets)
    (message `/Game/Primer/Primer_Shared/BPI_Activation.Trigger Activate` (`|GetArrayItem` _stagger_targets) self)
    (`KismetArrayLibrary.Array_Remove` (`self.Stagger Targets`))
    (`KismetSystemLibrary.Delay` 0.02)
    (`self.Stagger Activate`)))

(event `Handle Loops`
  (bind (_loop_count_min_max_x _loop_count_min_max_y) (`KismetMathLibrary.BreakVector2D` (`self.Loop Count Min Max`)))
  (bind _output_get (set `self.Num Loops` (`KismetMathLibrary.Round` (`KismetMathLibrary.RandomFloatInRange` _loop_count_min_max_x _loop_count_min_max_y))))
  (if (> _output_get 0)
    (bind _returnvalue (`KismetSystemLibrary.K2_SetTimerDelegate` (delegate `Trigger Loop`) (`self.Loop Interval`) true))
    (set `self.Loop Handle` _returnvalue)))

(event `Trigger Loop`
  (`self.Trigger`)
  (bind _result (`/Engine/EditorBlueprintResources/StandardMacros.DecrementInt` (`self.Num Loops`))
    (:`  `
      (if (<= _result 0)
        (`KismetSystemLibrary.K2_ClearAndInvalidateTimerHandle` (`self.Loop Handle`))))))

(event `Handle Disable Duration`
  (bind _max_disables (`self.Max Disables`))
  (`/Engine/EditorBlueprintResources/StandardMacros.IsValid` self
    (:`Is Valid`
      (if (> _max_disables -1)
        (bind _result (`/Engine/EditorBlueprintResources/StandardMacros.DecrementInt` _max_disables)
          (:`  `
            (if (< _result 0)
              (`self.K2_DestroyActor`)
              (else
                (if (> (`self.Disable Duration`) 0.0) :!label _label
                  (`PrimitiveComponent.SetCollisionEnabled` (`self.CollisionComponent`) "NoCollision")
                  (`KismetSystemLibrary.Delay` (`KismetMathLibrary.FMax` (`self.Disable Duration`) 0.2))
                  (`PrimitiveComponent.SetCollisionEnabled` (`self.CollisionComponent`) "QueryOnly"))))))
        (else
          (goto _label))))))

(fn `Handle Overlap`
  (params (InputPin :type "Actor Object Reference"))
  (locals (`L Triggered` :type Boolean :default false))
  (`/Engine/EditorBlueprintResources/ActorMacros.Switch Has Authority`
    (:`Authority`
      (for _array_element (`self.Allowed Trigger Class`)
        (if (`KismetMathLibrary.ClassIsChildOf` (`GameplayStatics.GetObjectClass` InputPin) _array_element)
          (`self.Trigger`)
          (`self.Handle Loops`)
          (`self.Handle Disable Duration`)
          (return))))))

(fn `Init Stagger Targets`
  (bind _activate_targets (`self.Activate Targets`))
  (if (!= (`self.All Actors with Tag`) "None")
    (for _array_element (`self.Activate Classes`)
      (bind _outactors (`GameplayStatics.GetAllActorsOfClassWithTag` _array_element (`self.All Actors with Tag`)))
      (for _array_element_2 _outactors
        (`KismetArrayLibrary.Array_AddUnique` (`self.Activate Targets`) _array_element_2))
      (if (> (`self.Max Count`) 0)
        (`KismetArrayLibrary.Array_Shuffle` _activate_targets)
        (`KismetArrayLibrary.Array_Resize` _activate_targets (`KismetMathLibrary.Min` (`KismetArrayLibrary.Array_Length` _activate_targets) (`self.Max Count`)))))
    (set `self.Stagger Targets` (`self.Activate Targets`))
    (else
      (set `self.Stagger Targets` (`self.Activate Targets`)))))

(fn `UserConstructionScript`)