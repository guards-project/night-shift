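; Spike trap Blueprint that raises and lowers a spear mesh when its inherited active state changes.
; On authority, a change resets a timer that plays the Trap timeline shortly after activation or reverses it after a longer delay, with start/stop cues via MCSound.
; The timeline lerps the mesh's height and plays a spike sound once per run using a DoOnce.
; The state-based cosmetic sound branch is an empty stub.
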(event `Start Anim`
  ;[1 1 1] One time sounds and events that occur at the moment of occurence (not late joiners)
  (`TimelineComponent.Play` (`self.Trap`)))

(event `self.On Active Changed`
  (params (Active :type Boolean))
  (`parent.On Active Changed` Active)
  (`|ExecutionSequence`
    (:`then_0`
      (`/Engine/EditorBlueprintResources/ActorMacros.Switch Has Authority`
        (:`Authority`
          (`KismetSystemLibrary.K2_ClearAndInvalidateTimerHandle` (`self.Timer Handle`))
          (if Active
            ;[1 1 1] One time sounds and events that occur at the moment of occurence (not late joiners)
            (bind _returnvalue (`KismetSystemLibrary.K2_SetTimerDelegate` (delegate `Start Anim`) 0.2))
            (set `self.Timer Handle` _returnvalue)
            (`self.MC Sound` "/Game/_Guards/Audio/Sounds/A_TrapStart_Cue.A_TrapStart_Cue")
            (else
              (bind _returnvalue_2 (`KismetSystemLibrary.K2_SetTimerDelegate` (delegate `Stop Anim`) 2.0))
              (set `self.Timer Handle` _returnvalue_2)
              (`self.MC Sound` "/Game/_Guards/Audio/Sounds/A_TrapStop_Cue.A_TrapStop_Cue"))))))
    (:`then_1`
      ;[1 1 1] State based sound control
      (`/Engine/EditorBlueprintResources/StandardMacros.Can Execute Cosmetic Events`
        (:`True`
          (if (`self.Active`)
            _))))))

(event `Stop Anim`
  ;[1 1 1] One time sounds and events that occur at the moment of occurence (not late joiners)
  (`TimelineComponent.Reverse` (`self.Trap`)))

(event `MC Sound`
  (params (Sound :type "SoundBase Object Reference"))
  (`GameplayStatics.PlaySoundAtLocation` Sound (`self.K2_GetActorLocation`) (struct) 1.0 1.0 0.0 null null null null))

(fn `UserConstructionScript`
  (`parent.UserConstructionScript`))