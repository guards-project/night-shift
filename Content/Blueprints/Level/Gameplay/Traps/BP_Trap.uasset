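; BP_Trap is a trap actor, apparently a base for variants, that activates while any Pawn overlaps its Box.
; The server sets the replicated Active flag, whose RepNotify calls OnActiveChanged, an empty hook for trap behavior.
; On BeginPlay, the server binds to DealtDamage on child-actor BP_DamageVolumes.
; When Force is positive, damaged Characters are launched away from the dealer with a vertical bias.
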(event `self.ReceiveBeginPlay`
  (`/Engine/EditorBlueprintResources/ActorMacros.Switch Has Authority`
    (:`Authority`
      (`self.Bind to Damage Dealt`))))

(event `self.Box.OnComponentBeginOverlap`
  (params (OverlappedComponent :type "PrimitiveComponent Object Reference") (OtherActor :type "Actor Object Reference") (OtherComp :type "PrimitiveComponent Object Reference") (OtherBodyIndex :type Integer) (bFromSweep :type Boolean) (SweepResult :type "HitResult Structure (by ref)"))
  (`/Engine/EditorBlueprintResources/ActorMacros.Switch Has Authority`
    (:`Authority`
      (`self.Check Activate`))))

(event `self.Box.OnComponentEndOverlap`
  (params (OverlappedComponent :type "PrimitiveComponent Object Reference") (OtherActor :type "Actor Object Reference") (OtherComp :type "PrimitiveComponent Object Reference") (OtherBodyIndex :type Integer))
  (`/Engine/EditorBlueprintResources/ActorMacros.Switch Has Authority`
    (:`Authority`
      (`self.Check Activate`))))

(event `Bind to Damage Dealt`
  (`/Engine/EditorBlueprintResources/ActorMacros.Switch Has Authority`
    (:`Authority`
      (for _array_element (`SceneComponent.GetChildrenComponents` (`self.DefaultSceneRoot`) true)
        (bind _aschild_actor_component (cast `ChildActorComponent` _array_element))
        (bind _asbp_damage_volume (cast `/Game/Blueprints/Level/Gameplay/BP_DamageVolume` (`ChildActorComponent.ChildActor` _aschild_actor_component)))
        (add `/Game/Blueprints/Level/Gameplay/BP_DamageVolume.Dealt Damage` _asbp_damage_volume (delegate `Dealt Damage_Event`))))))

(event `Dealt Damage_Event`
  (params (Dealer :type "Actor Object Reference") (`Damaged Actor` :type "Actor Object Reference") (Hit :type "HitResult Structure"))
  (if (> (`self.Force`) 0.0)
    (bind _ascharacter (cast `Character` `Damaged Actor`))
    (`Character.LaunchCharacter` _ascharacter (* (+ (`KismetMathLibrary.GetDirectionUnitVector` (`self.K2_GetActorLocation` Dealer) (`self.K2_GetActorLocation` `Damaged Actor`)) (`KismetMathLibrary.MakeVector` 0.0 0.0 (`self.Force Z Bias`))) (`self.Force`)) true true)))

(fn `Check Activate`
  (`self.Set Active` (`KismetArrayLibrary.Array_IsNotEmpty` (`PrimitiveComponent.GetOverlappingActors` (`self.Box`) "/Script/Engine.Pawn"))))

(fn `On Active Changed`
  (params (Active :type Boolean)))

(fn `OnRep_Active`
  (`self.On Active Changed` (`self.Active`)))

(fn `Set Active`
  (params (Active :type Boolean))
  (if (!= Active (`self.Active`))
    (set `self.Active` Active)))

(fn `UserConstructionScript`)