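; Small spinning saw blade trap that reacts to its parent's active state changes.
; On activation the authority starts the Spin timeline after a short delay, replaying it while active so the blade completes its current turn when switched off.
; One-shot start and stop sounds are multicast from the authority, while the looping spin sound fades with state on cosmetic-capable instances so late joiners hear it correctly.
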(event `self.On Active Changed`
  (params (Active :type Boolean))
  (`parent.On Active Changed` Active)
  (`|ExecutionSequence`
    (:`then_0`
      (`/Engine/EditorBlueprintResources/ActorMacros.Switch Has Authority`
        (:`Authority`
          ;[1 1 1] One shots, MC because we don't want it played ONREP for late joiners
          (`KismetSystemLibrary.K2_ClearAndInvalidateTimerHandle` (`self.Timer Handle`))
          (if Active
            (bind _returnvalue (`KismetSystemLibrary.K2_SetTimerDelegate` (delegate `Start Anim`) 0.5))
            (set `self.Timer Handle` _returnvalue)
            (`self.MC Sound` "/Game/_Guards/Audio/Sounds/A_TrapStart_Cue.A_TrapStart_Cue")
            (else
              (`self.MC Sound` "/Game/_Guards/Audio/Sounds/A_TrapStop_Cue.A_TrapStop_Cue"))))))
    (:`then_1`
      ;[1 1 1] State based sound (late joiner)
      (`/Engine/EditorBlueprintResources/StandardMacros.Can Execute Cosmetic Events`
        (:`True`
          (if (`self.Active`)
            (`AudioComponent.FadeIn` (`self.BladeSpinSound`) 0.5 1.0 0.0 "Linear")
            (else
              (`AudioComponent.FadeOut` (`self.BladeSpinSound`) 0.5 0.0 "Linear"))))))))

(event `Start Anim`
  ;[1 1 1] One shots, MC because we don't want it played ONREP for late joiners
  (`TimelineComponent.PlayFromStart` (`self.Spin`)))

(event `MC Sound`
  (params (Sound :type "SoundBase Object Reference"))
  (`GameplayStatics.PlaySoundAtLocation` Sound (`self.K2_GetActorLocation`) (struct) 1.0 1.0 0.0 null null null null))

(fn `UserConstructionScript`
  (`parent.UserConstructionScript`))