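; Swinging blade trap, built on a parent trap class, that swings its blade mesh back and forth while active.
; Activation plays a start cue and starts the Trap timeline after a short timer; deactivation cancels the timer and plays a stop cue.
; The timeline lerps blade rotation and triggers direction-filtered swipe sounds at the damage volume.
; At each end, the authority reverses the swing if still active, otherwise halts with a reset sound.
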(event `self.On Active Changed`
  (params (Active :type Boolean))
  (`parent.On Active Changed` Active)
  (`KismetSystemLibrary.K2_ClearAndInvalidateTimerHandle` (`self.Timer Handle`))
  (if Active
    (bind _returnvalue (`KismetSystemLibrary.K2_SetTimerDelegate` (delegate `Start Anim`) 0.5))
    (set `self.Timer Handle` _returnvalue)
    (`self.MC Sound` "/Game/_Guards/Audio/Sounds/A_TrapStart_Cue.A_TrapStart_Cue")
    (else
      (`self.MC Sound` "/Game/_Guards/Audio/Sounds/A_TrapStop_Cue.A_TrapStop_Cue"))))

(event `Start Anim`
  (`TimelineComponent.Play` (`self.Trap`)))

(event `MC Sound`
  (params (Sound :type "SoundBase Object Reference"))
  (`GameplayStatics.PlaySoundAtLocation` Sound (`self.K2_GetActorLocation`) (struct) 1.0 1.0 0.0 null null null null))

(event `MC Reset`
  (`/Engine/EditorBlueprintResources/StandardMacros.DoOnce` false :!via `Reset`
    (:`Completed`
      (`GameplayStatics.PlaySoundAtLocation` "/Game/Blueprints/Level/Gameplay/Traps/A_Spikes_Cue.A_Spikes_Cue" (`self.K2_GetActorLocation`) (struct) 1.0 1.0 0.0 null null null null))))

(fn `UserConstructionScript`
  (`parent.UserConstructionScript`))