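; Level-placed spawn marker that spawns random actors from a class list, giving Polygon AI a path node and a chance-weighted data table config.
; BeginPlay, player joins and Game.MinBalance changes trigger a one-time chance roll, gated to server or standalone and required player count.
; A successful roll spawns after an optional delay and repeats at intervals up to Count.
; Construction shows an editor preview, removed at runtime, and tags AI markers EnemySpawner.
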(event `self.ReceiveBeginPlay`
  (`|ExecutionSequence`
    (:`then_0`
      (`self.Trigger`)
      (`CVarChangeListenerManager.AddIntCVarCallbackStatic` "Game.MinBalance" (delegate `Balancing Changed`))
      (`self.Bind to Player Count Changed`))
    (:`then_1`
      (`self.Cleanup`))))

(event `Balancing Changed`
  (params (NewValue :type Integer))
  (if (>= NewValue (`self.Required Player Count`))
    (`self.Trigger`)))

(event `Trigger`
  (bind _spawn_delay (`self.Spawn Delay`))
  (if (`self.Can Execute Logic`)
    (`/Engine/EditorBlueprintResources/StandardMacros.DoOnce` false
      (:`Completed`
        (if (`KismetArrayLibrary.Array_IsValidIndex` (`self.Actor`))
          (`|ExecutionSequence`
            (:`then_1`
              (if (<= (`KismetMathLibrary.RandomFloat`) (`self.Chance to Spawn`))
                (if (>= _spawn_delay 0.0)
                  (if (== _spawn_delay 0.0)
                    (`self.Spawn Actor`)
                    (else
                      (`KismetSystemLibrary.K2_SetTimerDelegate` (`|CreateDelegate` :!event `Spawn Actor`) _spawn_delay))))))))))))

(event `/Game/Primer/Primer_Shared/BPI_Activation.Trigger Activate`
  (params (Context :type "Object Object Reference"))
  (if (`self.Can Execute Logic`)
    (`self.Spawn Actor`)))

(event `Delay Spawn`
  (params (Time :type "Float (single-precision)"))
  (`KismetSystemLibrary.K2_SetTimerDelegate` (`|CreateDelegate` :!event `Spawn Actor`) Time))

(event `Bind to Player Count Changed`
  (`/Engine/EditorBlueprintResources/ActorMacros.Switch Has Authority`
    (:`Authority`
      (bind _asbp_game_mode_template (cast `/Game/Blueprints/Core/BP_GameMode_Template` (`GameplayStatics.GetGameMode`)))
      (add `/Game/Blueprints/Core/Components/BP_PlayerJoinLeaveCallback.Player Joined` (`/Game/Blueprints/Core/BP_GameMode_Template.BP_PlayerJoinLeaveCallback` _asbp_game_mode_template) (delegate `Player Joined_Event`)))))

(event `Player Joined_Event`
  (params (Controller :type "Controller Object Reference") (PlayerState :type "PlayerState Object Reference"))
  (`KismetSystemLibrary.Delay` 0.2)
  (`self.Trigger`))

(event `On Spawned`
  (bind _result (`/Engine/EditorBlueprintResources/StandardMacros.IncrementInt` (`self.Current Count`))
    (:`  `
      (if (< _result (`self.Count`))
        (`KismetSystemLibrary.Delay` (`self.Interval`))
        (`self.Spawn Actor`) ; don't call trigger\nbecause the only way we reached here\nwas by Trigger randomly chancing a spawn\nso we should complete the desired count\notherwise we re-run chances each loop and\nnever end up with the defined count
      ))))

(fn `Can Execute Logic`
  (returns (ReturnValue :type Boolean))
  (bind _required_player_count (`self.Required Player Count`))
  ;[1 1 1] Required because Dungeons are loaded instance levels on clients, who believe they are authority
  (return (and (or (`KismetSystemLibrary.IsServer`) (`KismetSystemLibrary.IsStandalone`)) (or (>= (`KismetArrayLibrary.Array_Length` (`GameStateBase.PlayerArray` (`GameplayStatics.GetGameState`))) _required_player_count) (>= (`ConsoleUtils.GetIntCVar` "Game.MinBalance") _required_player_count)))))

(fn `Cleanup`
  (`|ExecutionSequence`
    (:`then_0`
      (bind _skeletalmesh (`self.SkeletalMesh`)
        (:`then`
          (`ActorComponent.K2_DestroyComponent` _skeletalmesh))
        (:`else`)))
    (:`then_1`
      (bind _childactor (`self.ChildActor`)
        (:`then`
          (`|ExecutionSequence`
            (:`then_0`
              (bind _childactor_2 (`ChildActorComponent.ChildActor` _childactor)
                (:`then`
                  (`self.K2_DestroyActor` _childactor_2))
                (:`else`)))
            (:`then_1`
              (`ActorComponent.K2_DestroyComponent` _childactor))))
        (:`else`)))))

(fn `Get Data Row`
  (returns (`Data Table Row` :type "DataTableRowHandle Structure"))
  (locals (`L Max` :type Integer) (`L Chosen` :type Integer :default 0) (`L Rows` :type "Array of DataTableRowHandle Structure"))
  (if (`KismetArrayLibrary.Array_IsValidIndex` (`self.Random Data Table Row`))
    (for _array_element (`self.Random Data Table Row`)
      (bind (_handle _chance) (break `/Game/Blueprints/Level/Gameplay/F_RandomRowConfig` _array_element))
      (for _ (range _chance)
        (`KismetArrayLibrary.Array_Add` (`local.L Rows`) _handle)))
    (if (`KismetArrayLibrary.Array_IsValidIndex` (`local.L Rows`))
      (return (`KismetArrayLibrary.Array_Random` (`local.L Rows`)))
      (else
        (return (`self.Data Table Row`))))
    (else
      (return (`self.Data Table Row`)))))

(fn `Refresh Editor Visual`
  (locals (`L Visual Class` :type "Actor Class Reference"))
  (bind _childactor (`self.ChildActor`))
  (bind (_datatable _rowname) (break `DataTableRowHandle` (`self.Get Data Row`)))
  (bind _outitem (`KismetArrayLibrary.Array_Random` (`self.Actor`)))
  (`/Engine/EditorBlueprintResources/StandardMacros.IsValid` (`GameplayStatics.GetGameInstance`) ; if not valid, is editor time
    (:`Is Valid`
      (bind _childactor_2 (`self.ChildActor`)
        (:`then`
          (`ChildActorComponent.SetChildActorClass` _childactor_2 null))
        (:`else`)))
    (:`Is Not Valid`
      (`self.SkeletalMesh`
        (:`then`
          (set `local.L Visual Class` _outitem)
          (if (`KismetSystemLibrary.IsValidClass` (`local.L Visual Class`))
            (if (`KismetMathLibrary.ClassIsChildOf` _outitem "/Game/Blueprints/Core/PolygonAI/BP_Polygon_AI.BP_Polygon_AI_C")
              (`/Engine/EditorBlueprintResources/StandardMacros.IsValid` _datatable
                (:`Is Valid`
                  (bind _returnvalue (`|GetDataTableRow` _datatable _rowname)
                    (:`then`
                      (bind _returnvalue_2 (`KismetSystemLibrary.LoadAsset_Blocking` (`KismetArrayLibrary.Array_Random` (`.Skin_44_CC605ABF4AEA3B2F3C686EA32C0D8727` (break `/Game/Blueprints/Core/PolygonAI/Config/F_Character_Setup` _returnvalue)))))
                      (bind _asskeletal_mesh (cast `SkeletalMesh` _returnvalue_2))
                      (`SkinnedMeshComponent.SetSkinnedAssetAndUpdate` (`self.SkeletalMesh`) _asskeletal_mesh true)
                      (`SceneComponent.SetVisibility` (`self.SkeletalMesh`) true false))))
                (:`Is Not Valid`
                  (`SceneComponent.SetVisibility` (`self.SkeletalMesh`) false false :!label _label)))
              (else
                (`SceneComponent.SetVisibility` (`self.SkeletalMesh`) false false)
                (if (!= (`ChildActorComponent.ChildActorClass` _childactor) (`local.L Visual Class`))
                  (`ChildActorComponent.SetChildActorClass` _childactor (`local.L Visual Class`)))))
            (else
              (goto _label))))
        (:`else`)))))

(fn `Spawn Actor`
  (locals (`L Class` :type "Actor Class Reference"))
  (bind _returnvalue (`self.GetTransform`))
  (if (`KismetArrayLibrary.Array_IsValidIndex` (`self.Actor`))
    (bind _output_get (set `local.L Class` (`KismetArrayLibrary.Array_Random` (`self.Actor`))))
    (bind _asbp_polygon_ai (castclass `/Game/Blueprints/Core/PolygonAI/BP_Polygon_AI` _output_get)
      (:`then`
        (bind _returnvalue_2 (`|SpawnActorFromClass` _asbp_polygon_ai (`KismetMathLibrary.MakeTransform` (+ (.location _returnvalue) (0.0 0.0 90.0)) (.rotation _returnvalue) (.scale _returnvalue)) "AdjustIfPossibleButAlwaysSpawn" "SelectDefaultAtRuntime" null (`self.Path Node`) (`self.Get Data Row`) null))
        (`/Engine/EditorBlueprintResources/StandardMacros.IsValid` _returnvalue_2
          (:`Is Valid`
            (bind _output_get_2 (set `self.Last Spawned Actor` _returnvalue_2))
            (`self.Actor Spawned` self _output_get_2)
            (`self.On Spawned`))))
      (:`CastFailed`
        (bind _returnvalue_3 (`|SpawnActorFromClass` (`local.L Class`) _returnvalue "AdjustIfPossibleButAlwaysSpawn" "SelectDefaultAtRuntime" null null))
        (`/Engine/EditorBlueprintResources/StandardMacros.IsValid` _returnvalue_3
          (:`Is Valid`
            (`self.Actor Spawned` self _returnvalue_3)
            (`self.On Spawned`)))))))

(fn `Update Tags`
  (for _array_element (`self.Actor`)
    (if (`KismetMathLibrary.ClassIsChildOf` _array_element "/Game/Blueprints/Core/PolygonAI/BP_Polygon_AI.BP_Polygon_AI_C")
      (`KismetArrayLibrary.Array_AddUnique` (`self.Tags`) "EnemySpawner")
      (return)))
  (`KismetArrayLibrary.Array_RemoveItem` (`self.Tags`) "EnemySpawner"))

(fn `UserConstructionScript`
  (`self.Refresh Editor Visual`)
  (`self.Update Tags`))