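; BP_EnemyCloset is a level gameplay actor linked to enemy spawners that lets spawned characters move through it.
; On BeginPlay, the server binds to each valid spawner's ActorSpawned event and sets each spawned character template's capsule to ignore the closet when moving.
; TriggerActivate intentionally leaves the spawners untriggered, as a comment notes the repop tag already makes them spawn.
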(event `/Game/Primer/Primer_Shared/BPI_Activation.Trigger Activate`
  (params (Context :type "Object Object Reference"))
  ;[1 1 1] dont trigger the spawners, repop tag will already make them spawn
)

(event `self.ReceiveBeginPlay`
  (`/Engine/EditorBlueprintResources/ActorMacros.Switch Has Authority`
    (:`Authority`
      (for _array_element (`self.Enemy Spawners`)
        (`/Engine/EditorBlueprintResources/StandardMacros.IsValid` _array_element
          (:`Is Valid`
            (add `/Game/Blueprints/Level/Gameplay/BP_GameplayMarker.Actor Spawned` _array_element (delegate `Actor Spawned_Event`))))))))

(event `Actor Spawned_Event`
  (params (Invoker :type "/Game/Blueprints/Level/Gameplay/BP_GameplayMarker Object Reference") (`Spawned Actor` :type "Actor Object Reference"))
  (bind _asbp_character_template (cast `/Game/Blueprints/Core/BP_Character_Template` `Spawned Actor`))
  (`PrimitiveComponent.IgnoreActorWhenMoving` (`Character.CapsuleComponent` _asbp_character_template) self true))

(fn `UserConstructionScript`)