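; Damage volume that hurts actors on overlap and can pin killed characters to itself.
; While active, the server applies an optional gameplay effect and point damage, then plays a flesh-hit sound.
; When sticky, it spawns a physics constraint from a dead character's nearest bone to its collision, removed after a duration or on revival.
; Both trigger activate and deactivate events switch the volume off.
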(event `self.CollisionComponent.OnComponentBeginOverlap`
  (params (OverlappedComponent :type "PrimitiveComponent Object Reference") (OtherActor :type "Actor Object Reference") (OtherComp :type "PrimitiveComponent Object Reference") (OtherBodyIndex :type Integer) (bFromSweep :type Boolean) (SweepResult :type "HitResult Structure (by ref)"))
  (`/Engine/EditorBlueprintResources/ActorMacros.Switch Has Authority`
    (:`Authority`
      (if (`self.Active`)
        (`self.Deal Damage` OtherActor SweepResult)))))

(event `/Game/Primer/Primer_Shared/BPI_Activation.Trigger Activate`
  (params (Context :type "Object Object Reference"))
  (`self.Set Active` false))

(event `/Game/Primer/Primer_Shared/BPI_Activation.Trigger Deactivate`
  (params (Context :type "Object Object Reference"))
  (`self.Set Active` false))

(event `MC Sound`
  (params (Sound :type "SoundBase Object Reference"))
  (`GameplayStatics.PlaySoundAtLocation` Sound (`self.K2_GetActorLocation`) (struct) 1.0 1.0 0.0 null null null null))

(fn `Apply Effect`
  (params (Target :type "Actor Object Reference"))
  (bind _gameplay_effect_class (`self.Gameplay Effect Class`)
    (:`then`
      (`AbilitySystemComponent.BP_ApplyGameplayEffectToSelf` :`self` (`AbilitySystemBlueprintLibrary.GetAbilitySystemComponent` Target) :`GameplayEffectClass` _gameplay_effect_class))
    (:`else`)))

(fn `Can Constrain`
  (params (Character :type "Character Object Reference")))

(fn `Create Attachment`
  (params (Character :type "/Game/Blueprints/Core/BP_Character_Template Object Reference"))
  (locals (`L Bone` :type Name) (`Other Comp` :type "PrimitiveComponent Object Reference"))
  (bind _character (`local.Character`))
  (bind _character_2 (`local.Character`))
  ;[1 1 1] Nearest Bone
  (set `local.L Bone` (`.ReturnValue` (`SkinnedMeshComponent.FindClosestBone_K2` (`Character.Mesh` (`local.Character`)) (`self.K2_GetActorLocation`) 0.0 true)))
  (`/Game/Blueprints/Core/BP_Character_Template.Remove Death Constraint` _character_2)
  (add `/Game/Blueprints/Core/BP_Character_Template.OnRevived` _character_2 (`|CreateDelegate` :!event `On Revived`)) ; remove physics constraints after revival
  (bind _returnvalue (`|SpawnActorFromClass` "/Game/Blueprints/Items/Ranged/BP_Constraint.BP_Constraint_C" (`self.GetTransform`) "AlwaysSpawn" "OverrideRootScale" self (make `/Game/Blueprints/Items/Ranged/F_Constraint` (`Character.Mesh` (`local.Character`)) (`local.L Bone`) (`self.CollisionComponent`)) false null)) ; spawn a constraint that constrains the character mesh to this projectile
  (`KismetArrayLibrary.Array_Add` (`self.Constraint`) _returnvalue)
  (`self.K2_AttachToActor` _returnvalue self "None" "SnapToTarget" "SnapToTarget" "KeepRelative" true) ; attach the constraint to this projectile so they move together
  (`/Game/Blueprints/Core/BP_Character_Template.Track Constraint` _character _returnvalue)
  (`/Game/Blueprints/Core/BP_Character_Template.Delay Remove Constraints` _character (`self.Sticky Duration`)))

(fn `Deal Damage`
  (params (DamagedActor :type "Actor Object Reference") (Hit :type "HitResult Structure (by ref)"))
  (`self.Dealt Damage` self DamagedActor Hit)
  (`self.Apply Effect` DamagedActor)
  (`GameplayStatics.ApplyPointDamage` DamagedActor (`self.Damage`) (`.Normal` (`GameplayStatics.BreakHitResult` Hit)) Hit null self (`self.Damage Type Class`))
  (`self.MC Sound` "/Game/Blueprints/GAS/Cues/Sounds/HitFlesh/A_Hit_Flesh.A_Hit_Flesh")
  (if (`self.Sticky`)
    (bind _dead (message `/Game/Blueprints/Core/BPI_Character.Is Dead` DamagedActor))
    (if _dead
      (bind _asbp_character_template (cast `/Game/Blueprints/Core/BP_Character_Template` (`local.DamagedActor`)))
      (bind _returnvalue (`KismetArrayLibrary.Array_AddUnique` (`self.Already Constrained`) _asbp_character_template))
      (if (>= _returnvalue 0)
        (`self.Create Attachment` _asbp_character_template)))))

(fn `On Attachment Updated`
  (bind (_root_attachment_component _root_attachment_bone _root_attachment_relativetransform) (break `/Game/Blueprints/Items/Ranged/F_Attach` (`self.Root Attachment`)))
  (bind _root_attachment_component_2 (break `/Game/Blueprints/Items/Ranged/F_Attach` (`self.Root Attachment`)))
  (bind (_component _bone) (break `/Game/Blueprints/Items/Ranged/F_Attach` (`self.Root Attachment`)))
  ;[1 1 1] Become static (don't cause overlaps, only interactable)
  (`/Engine/EditorBlueprintResources/StandardMacros.IsValid` (`.Component_16_7179BA4B403648FB10CC738584E38CE8` (break `/Game/Blueprints/Items/Ranged/F_Attach` (`self.Root Attachment`)))
    (:`Is Valid`
      (`PrimitiveComponent.IgnoreActorWhenMoving` _root_attachment_component_2 self true)
      ;[1 1 1] Attach after disabling
      (`self.K2_AttachToComponent` _component _bone "SnapToTarget" "KeepWorld" "KeepWorld")
      (`self.K2_SetActorRelativeTransform` _root_attachment_relativetransform))))

(fn `On Revived`
  (params (Actor :type "/Game/Blueprints/Core/BP_Character_Template Object Reference"))
  (bind (_arrayindex _arrayelement) (`/Engine/EditorBlueprintResources/StandardMacros.ReverseForEachLoop` (`self.Constraint`))
    (:`LoopBody`
      (`/Engine/EditorBlueprintResources/StandardMacros.IsValid` _arrayelement
        (:`Is Valid`
          (`self.K2_DestroyActor` _arrayelement)
          (`KismetArrayLibrary.Array_Remove` (`self.Constraint`) _arrayindex))))))

(fn `OnRep_Root Attachment`
  (`self.On Attachment Updated`))

(fn `Set Active`
  (params (Active :type Boolean))
  (set `self.Active` Active))

(fn `UserConstructionScript`)