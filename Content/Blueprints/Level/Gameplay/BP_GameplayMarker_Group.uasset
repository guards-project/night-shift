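; BP_GameplayMarker_Group is a level marker group that activates a random selection of its attached actors, typically gameplay markers.
; On BeginPlay or balance CVar changes, a server/standalone check gated by player count or Game.MinBalance leads to a one-time chance roll with optional delay.
; TriggerActivate skips the roll and delay; an optional authority binding retries on player joins.
; Spawn events from selected markers are relayed through the group's GroupSpawnedActor dispatcher.
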(event `self.ReceiveBeginPlay`
  (`self.Trigger`)
  (`CVarChangeListenerManager.AddIntCVarCallbackStatic` "Game.MinBalance" (delegate `Balancing Changed`)))

(event `Balancing Changed`
  (params (NewValue :type Integer))
  (if (>= NewValue (`self.Required Player Count`))
    (`self.Trigger`)))

(event `Trigger`
  (bind _spawn_delay (`self.Spawn Delay`))
  (if (`self.Can Execute Logic`)
    (`/Engine/EditorBlueprintResources/StandardMacros.DoOnce` false
      (:`Completed`
        (if (<= (`KismetMathLibrary.RandomFloat`) (`self.Chance to Trigger`))
          (if (>= _spawn_delay 0.0)
            (if (== _spawn_delay 0.0)
              (`self.Trigger Child Actors`)
              (else
                (`KismetSystemLibrary.K2_SetTimerDelegate` (`|CreateDelegate` :!event `Trigger Child Actors`) _spawn_delay)))))))))

(event `/Game/Primer/Primer_Shared/BPI_Activation.Trigger Activate`
  (params (Context :type "Object Object Reference"))
  (if (`self.Can Execute Logic`)
    (`self.Trigger Child Actors`)))

(event `Bind to Player Count Changed`
  (`/Engine/EditorBlueprintResources/ActorMacros.Switch Has Authority`
    (:`Authority`
      (bind _asbp_game_mode_template (cast `/Game/Blueprints/Core/BP_GameMode_Template` (`GameplayStatics.GetGameMode`)))
      (add `/Game/Blueprints/Core/Components/BP_PlayerJoinLeaveCallback.Player Joined` (`/Game/Blueprints/Core/BP_GameMode_Template.BP_PlayerJoinLeaveCallback` _asbp_game_mode_template) (delegate `Player Joined_Event`)))))

(event `Player Joined_Event`
  (params (Controller :type "Controller Object Reference"))
  (`KismetSystemLibrary.Delay` 0.2)
  (`self.Trigger`))

(fn `Can Execute Logic`
  (returns (ReturnValue :type Boolean))
  (bind _returnvalue (`KismetArrayLibrary.Array_Length` (`GameStateBase.PlayerArray` (`GameplayStatics.GetGameState`))))
  ;[1 1 1] Required because Dungeons are loaded instance levels on clients, who believe they are authority
  (return (and (or (`KismetSystemLibrary.IsServer`) (`KismetSystemLibrary.IsStandalone`)) (or (>= _returnvalue (`self.Required Player Count`)) (>= (`ConsoleUtils.GetIntCVar` "Game.MinBalance") _returnvalue)))))

(fn `On Group Spawned Actor`
  (params (Invoker :type "/Game/Blueprints/Level/Gameplay/BP_GameplayMarker Object Reference") (`Spawned Actor` :type "Actor Object Reference"))
  (`self.Group Spawned Actor` self Invoker `Spawned Actor`))

(fn `Trigger Child Actors`
  (locals (`L Attached Actors` :type "Array of Actor Object Reference"))
  (bind _returnvalue (`KismetArrayLibrary.Array_Length` (`local.L Attached Actors`)))
  (bind _output_get (set `local.L Attached Actors` (`self.GetAttachedActors` true)))
  (`KismetArrayLibrary.Array_Shuffle` _output_get)
  (`KismetArrayLibrary.Array_Resize` (`local.L Attached Actors`) (`KismetMathLibrary.SelectInt` _returnvalue (`KismetMathLibrary.Min` (`KismetMathLibrary.RandomIntegerInRange` (`self.Min Count`) (`self.Max Count`)) _returnvalue) (<= (`self.Max Count`) 0)))
  (for _array_element (`local.L Attached Actors`)
    (bind _asbp_gameplay_marker (cast `/Game/Blueprints/Level/Gameplay/BP_GameplayMarker` _array_element))
    (add `/Game/Blueprints/Level/Gameplay/BP_GameplayMarker.Actor Spawned` _asbp_gameplay_marker (`|CreateDelegate` :!event `On Group Spawned Actor`)))
  (message `/Game/Primer/Primer_Shared/BPI_Activation.Trigger Activate` (`local.L Attached Actors`) self))

(fn `UserConstructionScript`)