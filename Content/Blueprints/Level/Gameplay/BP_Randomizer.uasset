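; BP_Randomizer is a level gameplay actor that randomly thins out placed actors of configured classes when play begins.
; On BeginPlay it gathers all actors of every listed class into one shared pool, then rolls a count within the KeepCount range, floored at one.
; It shuffles the pool and destroys actors with an index above that count, so one more than the rolled number survives.
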(event `self.ReceiveBeginPlay`
  (bind (_keep_count_x _keep_count_y) (`KismetMathLibrary.BreakVector2D` (`self.Keep Count`)))
  (for _array_element (`self.Class`)
    (bind _outactors (`GameplayStatics.GetAllActorsOfClass` _array_element))
    (`KismetArrayLibrary.Array_Append` (`self.Targets`) _outactors))
  (set `self.Desired Count` (`KismetMathLibrary.Max` (`KismetMathLibrary.FTrunc` (`KismetMathLibrary.RandomFloatInRange` _keep_count_x _keep_count_y)) 1))
  (`KismetArrayLibrary.Array_Shuffle` (`self.Targets`))
  (for (_array_element_2 _array_index) (`self.Targets`)
    (if (> _array_index (`self.Desired Count`))
      (`self.K2_DestroyActor` _array_element_2))))

(fn `UserConstructionScript`)