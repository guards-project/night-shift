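; Server-side level spawner that spawns requested counts of actor classes inside a box volume on BeginPlay, optionally delayed.
; Each request entry resolves its soft class, blocking-loading it if needed, then batches repeat after a delay, finitely or indefinitely per RepeatCount.
; SpawnActor traces down from a random box point, spawns at the hit with random yaw and slight scale variation, then broadcasts ActorSpawned.
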(event `self.ReceiveBeginPlay`
  (`/Engine/EditorBlueprintResources/ActorMacros.Switch Has Authority`
    (:`Authority`
      (`self.Init Spawning`))))

(event `Init Spawning`
  (bind _start_delay (`self.Start Delay`))
  ;[1 1 1] Init Spawning
  (if (> _start_delay 0.0)
    (`KismetSystemLibrary.Delay` _start_delay)
    (`self.Start Spawning`)
    (elif (== _start_delay 0.0)
      (`self.Start Spawning`))))

(event `Start Spawning`
  (bind _returnvalue (`KismetSystemLibrary.K2_SetTimerDelegate` (`|CreateDelegate` :!event `Process Spawn Request`) (`self.Repeat Delay`)))
  (set `self.Spawn Timer` _returnvalue)
  (`self.Process Spawn Request`))

(event `Stop Spawning`
  (bind _repeat_count (`self.Repeat Count`))
  (`KismetSystemLibrary.K2_ClearAndInvalidateTimerHandle` (`self.Spawn Timer`))
  (if (or (< _repeat_count 0) (and (> _repeat_count 0) (< (`self.Current Loop`) (`self.Repeat Count`))))
    (`KismetSystemLibrary.Delay` (`self.Repeat Delay`))
    (`/Engine/EditorBlueprintResources/StandardMacros.IncrementInt` (`self.Current Loop`)
      (:`  `
        (`self.Start Spawning`)))))

(event `Process Spawn Request`
  (for _array_element (`self.Request`)
    (bind (_class _count) (break `/Game/Blueprints/Level/F_SpawnRequest` _array_element))
    (bind _output (`|ConvertAsset` _class))
    (if (`KismetSystemLibrary.IsValidClass` _output)
      (for _ (range (+ _count 1))
        (`self.Spawn Actor` _output))
      (else
        (bind _returnvalue (`KismetSystemLibrary.LoadClassAsset_Blocking` _class))
        (bind _asactor (castclass `Actor` _returnvalue))
        (for _ (range (+ _count 1))
          (`self.Spawn Actor` _asactor)))))
  (`self.Stop Spawning`))

(fn `Spawn Actor`
  (params (Class :type "Actor Class Reference"))
  (locals (`L Rand Location in Box` :type "Vector Structure" :default (0.0 0.0 0.0)))
  (bind (_origin _boxextent) (`KismetSystemLibrary.GetComponentBounds` (`self.Box`)))
  (bind _output_get (set `local.L Rand Location in Box` (`KismetMathLibrary.RandomPointInBoundingBox` _origin _boxextent)))
  (bind (_outhit _returnvalue) (`KismetSystemLibrary.LineTraceSingle` :`Start` _output_get :`End` (- _output_get (`KismetMathLibrary.MakeVector` 0.0 0.0 (`self.Trace Depth`))) :`TraceChannel` "TraceTypeQuery1" :`DrawDebugType` "ForDuration"))
  (if _returnvalue
    (bind _returnvalue_2 (`|SpawnActorFromClass` (`local.Class`) (`KismetMathLibrary.MakeTransform` (+ (`.Location` (`GameplayStatics.BreakHitResult` _outhit)) (`KismetMathLibrary.MakeVector` 0.0 0.0 (`self.Trace End Z Offset`))) (`KismetMathLibrary.MakeRotator` 0.0 0.0 (`KismetMathLibrary.RandomFloatInRange` 0.0 360.0)) (`KismetMathLibrary.Conv_DoubleToVector` (`KismetMathLibrary.RandomFloatInRange` 1.0 1.2))) "AdjustIfPossibleButAlwaysSpawn" "OverrideRootScale" null null))
    (`self.Actor Spawned` self _returnvalue_2)
    (else
      (`KismetSystemLibrary.PrintString` (`KismetStringLibrary.Concat_StrStr` "Failed to spawn at" "" (`KismetStringLibrary.Conv_VectorToString` (`local.L Rand Location in Box`)))))))

(fn `UserConstructionScript`)