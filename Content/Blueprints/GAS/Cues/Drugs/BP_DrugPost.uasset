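; Drug effect actor in the GAS cues folder that shows a temporary post-process screen effect using a randomly chosen material.
; On BeginPlay it synchronously loads a random entry from Materials, makes a dynamic instance and adds it to the PostProcess component at full weight.
; A timeline, rate-scaled to span Duration, drives the material's Lerp parameter and destroys the actor when finished.
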(event `self.ReceiveBeginPlay`
  (bind _timeline (`self.Timeline`))
  (bind _returnvalue (`KismetSystemLibrary.LoadAsset_Blocking` (`KismetArrayLibrary.Array_Random` (`self.Materials`))))
  (bind _asmaterial_interface (cast `MaterialInterface` _returnvalue))
  (bind _returnvalue_2 (`KismetMaterialLibrary.CreateDynamicMaterialInstance` _asmaterial_interface))
  (set `self.Material` _returnvalue_2)
  (`TimelineComponent.SetPlayRate` _timeline (/ 1.0 (`self.Duration`)))
  (`TimelineComponent.PlayFromStart` _timeline)
  (`PostProcessComponent.AddOrUpdateBlendable` (`self.PostProcess`) (`self.Material`) 1.0))

(fn `UserConstructionScript`)