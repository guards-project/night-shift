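; Gameplay Ability that toggles the character's walk move state.
; On activation it commits, then on authority only casts the avatar to BP_Character_Template, flips MoveState between the first two enum values via AuthSetMoveState and ends.
; A failed commit cancels the ability, while non-authority execution and a failed cast never call EndAbility.
; Activation, commit failure, cancellation and completion print debug strings.
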(event `self.K2_ActivateAbility`
  (`KismetSystemLibrary.PrintString` "On Activate Walk Ability" true true (struct :`R` 1.0 :`G` 0.406657 :`A` 1.0))
  (bind _returnvalue (`self.K2_CommitAbility`))
  (if _returnvalue
    (`self.K2_HasAuthority`
      (:`True`
        (bind _asbp_character_template (cast `/Game/Blueprints/Core/BP_Character_Template` (`self.GetAvatarActorFromActorInfo`)))
        (`/Game/Blueprints/Core/BP_Character_Template.Auth Set Move State` _asbp_character_template (select `bool` (`|EnumEquality` (`/Game/Blueprints/Core/BP_Character_Template.Move State` _asbp_character_template) "NewEnumerator0") :`false` "NewEnumerator0" :`true` "NewEnumerator1" :!type "/Game/Blueprints/Core/E_MoveState Enum"))
        (`self.K2_EndAbility`)))
    (else
      (`self.K2_CancelAbility`)
      (`KismetSystemLibrary.PrintString` "Cannot Commit Walk"))))

(event `self.K2_OnEndAbility`
  (params (bWasCancelled :type Boolean))
  (if bWasCancelled
    (`KismetSystemLibrary.PrintString` "Ability Cancelled: Walk")
    (else
      (`KismetSystemLibrary.PrintString` "Ability Ended: Walk"))))