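; Gameplay ability for a directional dodge dash, allowed only while the avatar is shielding and moving away from straight ahead.
; After committing, it picks a root dodge montage from the angle and side of velocity relative to control yaw.
; Near-forward movement yields no montage and cancels.
; The ability ends as soon as the montage starts, leaving it playing; the activation check ignores the parent's boolean result.
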(event `self.K2_ActivateAbility`
  (`KismetSystemLibrary.PrintString` "On Activate Dash Ability" true true (struct :`R` 1.0 :`G` 0.406657 :`A` 1.0))
  (bind _returnvalue (`self.K2_CommitAbility`))
  (if _returnvalue
    (bind _dash_anim (`self.Dash`))
    (`/Engine/EditorBlueprintResources/StandardMacros.IsValid` _dash_anim
      (:`Is Valid`
        (`AbilityTask_PlayMontageAndWait.CreatePlayMontageAndWaitProxy` "None" _dash_anim 1.0 "None" false
          (:`then`
            (`self.K2_EndAbility`))))
      (:`Is Not Valid`
        (`self.K2_CancelAbility`)))
    (else
      (`self.K2_CancelAbility`)
      (`KismetSystemLibrary.PrintString` "Cannot Commit Dash"))))

(fn `Dash`
  (returns (`Dash Anim` :type "AnimMontage Object Reference"))
  (locals (`L Angle` :type "Float (double-precision)") (`L isRight` :type Boolean) (`L Anim` :type "AnimMontage Object Reference") (`L Character` :type "Character Object Reference"))
  (bind _l_angle (`local.L Angle`))
  (bind _ascharacter (cast `Character` (`self.GetAvatarActorFromActorInfo`)))
  (set `local.L Character` _ascharacter)
  (set `local.L Angle` (`self.Get Move Angle`))
  (set `local.L isRight` (> (`KismetMathLibrary.Dot_VectorVector` (`KismetMathLibrary.Normal` (`Actor.GetVelocity` (`self.GetAvatarActorFromActorInfo`))) (`KismetMathLibrary.GetRightVector` (`KismetMathLibrary.MakeRotator` 0.0 0.0 (.yaw (`Pawn.GetControlRotation` (`local.L Character`)))))) 0.0))
  (`|ExecutionSequence`
    (:`then_0`
      (if (< _l_angle 30.0)
        (return null)
        (elif (< _l_angle 70.0)
          (set `local.L Anim` (select `bool` (`local.L isRight`) :`false` "/Game/Polygon/Animations/PolygonAnims/Locomotion/DodgeForwardLeft_Root_Montage.DodgeForwardLeft_Root_Montage" :`true` "/Game/Polygon/Animations/PolygonAnims/Locomotion/DodgeForwardRight_Root_Montage.DodgeForwardRight_Root_Montage" :!type "AnimMontage Object Reference"))
          (elif (< (`local.L Angle`) 120.0)
            (set `local.L Anim` (select `bool` (`local.L isRight`) :`false` "/Game/Polygon/Animations/PolygonAnims/Locomotion/DodgeLeft_Root_Montage.DodgeLeft_Root_Montage" :`true` "/Game/Polygon/Animations/PolygonAnims/Locomotion/DodgeRight_Root_Montage.DodgeRight_Root_Montage" :!type "AnimMontage Object Reference"))
            (elif (< (`local.L Angle`) 170.0)
              (set `local.L Anim` (select `bool` (`local.L isRight`) :`false` "/Game/Polygon/Animations/PolygonAnims/Locomotion/DodgeBackwardLeft_Root_Montage.DodgeBackwardLeft_Root_Montage" :`true` "/Game/Polygon/Animations/PolygonAnims/Locomotion/DodgeBackwardRight_Root_Montage.DodgeBackwardRight_Root_Montage" :!type "AnimMontage Object Reference"))
              (else
                (set `local.L Anim` "/Game/Polygon/Animations/PolygonAnims/Locomotion/DodgeBackward_Root_Montage.DodgeBackward_Root_Montage")))))))
    (:`then_1`
      (return (`local.L Anim`)))))

(fn `Get Move Angle`
  (returns (ReturnValue :type "Float (double-precision)"))
  (bind _returnvalue (`self.GetAvatarActorFromActorInfo`))
  (`/Engine/EditorBlueprintResources/StandardMacros.IsValid` _returnvalue
    (:`Is Valid`
      (bind _ascharacter (cast `Character` _returnvalue))
      (return (`KismetMathLibrary.DegAcos` (`KismetMathLibrary.Dot_VectorVector` (`KismetMathLibrary.Normal` (`Actor.GetVelocity` (`self.GetAvatarActorFromActorInfo`))) (`KismetMathLibrary.GetForwardVector` (`KismetMathLibrary.MakeRotator` 0.0 0.0 (.yaw (`Pawn.GetControlRotation` _ascharacter))))))))))

(fn `K2_CanActivateAbility`
  (params (ActorInfo :type "GameplayAbilityActorInfo Structure") (Handle :type "GameplayAbilitySpecHandle Structure"))
  (returns (RelevantTags :type "GameplayTagContainer Structure") (ReturnValue :type Boolean))
  (bind _returnvalue (`self.GetAvatarActorFromActorInfo`))
  (bind _returnvalue_2 (and (`GSCBlueprintFunctionLibrary.HasAnyMatchingGameplayTag` _returnvalue (struct :`GameplayTags` (struct :`(TagName` "State.Shielding") :`(TagName` "State.Guarding")))) (> (`self.Get Move Angle`) 20.0) (> (`KismetMathLibrary.VSize` (`Actor.GetVelocity` _returnvalue)) 5.0)))
  (bind _relevanttags (`parent.K2_CanActivateAbility` ActorInfo Handle))
  (`/Engine/EditorBlueprintResources/StandardMacros.IsValid` _returnvalue
    (:`Is Valid`
      (`KismetSystemLibrary.PrintString` (`KismetStringLibrary.Conv_BoolToString` _returnvalue_2))
      (return _relevanttags _returnvalue_2))))