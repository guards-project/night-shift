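; GA_Crouch is a Gameplay Ability that toggles the avatar Character between crouched and standing.
; On activation it commits the ability, then, if the Character is locally controlled, calls Crouch or UnCrouch based on its crouched state and ends immediately.
; A failed commit cancels the ability, and debug strings are printed on activation, commit failure and end.
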(event `self.K2_ActivateAbility`
  (bind _character (`self.Character`))
  (`KismetSystemLibrary.PrintString` "On Activate Crouch Ability" true true (struct :`R` 1.0 :`G` 0.406657 :`A` 1.0))
  (bind _returnvalue (`self.K2_CommitAbility`))
  (if _returnvalue
    (bind _ascharacter (cast `Character` (`self.GetAvatarActorFromActorInfo`)))
    (if (`Pawn.IsLocallyControlled` _ascharacter)
      (set `self.Character` _ascharacter)
      (if (`Character.bIsCrouched` (`self.Character`))
        (`Character.UnCrouch` _character)
        (else
          (`Character.Crouch` _character)))
      (`self.K2_EndAbility`))
    (else
      (`self.K2_CancelAbility`)
      (`KismetSystemLibrary.PrintString` "Cannot Commit Crouch"))))

(event `self.K2_OnEndAbility`
  (params (bWasCancelled :type Boolean))
  (`KismetSystemLibrary.PrintString` (`KismetMathLibrary.SelectString` "Crouch Cancelled" "Crouch Ended" bWasCancelled)))