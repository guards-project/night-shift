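; Gameplay ability that, despite its Distract name, shouts a follow-or-stay command to nearby AI.
; Plays a pointing montage unless seated; the server then runs AOEFollowStay, multicasts a voice line and ends after a short delay.
; A sphere overlap makes leaderless unarrested civilians and arrested perps follow the player's controller, skipping any at the APC.
; Only when nobody new starts following are the player's current followers told to stop.
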(event `self.K2_ActivateAbility`
  (bind (_voice_line_datatable _voice_line_rowname) (break `DataTableRowHandle` (`self.Voice Line`)))
  (`KismetSystemLibrary.PrintString` "On Activate Distract Ability" true true (struct :`R` 1.0 :`G` 0.406657 :`A` 1.0))
  (bind _returnvalue (`self.K2_CommitAbility`))
  (if _returnvalue
    (bind _asbp_character_template (cast `/Game/Blueprints/Core/BP_Character_Template` (`self.GetAvatarActorFromActorInfo`)))
    (if (not (`/Game/Blueprints/Core/BP_Character_Template.Seated` _asbp_character_template))
      (`GSCTask_PlayMontageWaitForEvent.PlayMontageAndWaitForEvent` "None" "/Game/Polygon/Animations/PolygonAnims/Poses/AS_Polygon_Point_Montage.AS_Polygon_Point_Montage"
        (:`then`
          _)))
    (`self.K2_HasAuthority`
      (:`True`
        (`self.AOE Follow Stay`)
        (`/Game/_Guards/Audio/VoiceSet/BP_Voice_Component.MC Voice` (`Actor.GetComponentByClass` (`self.GetAvatarActorFromActorInfo`) "/Game/_Guards/Audio/VoiceSet/BP_Voice_Component.BP_Voice_Component_C") _voice_line_rowname)
        (`KismetSystemLibrary.Delay` 1.5)
        (`self.K2_EndAbility`)))
    (else
      (`self.K2_CancelAbility`)
      (`KismetSystemLibrary.PrintString` "Cannot Commit Crouch"))))

(event `self.K2_OnEndAbility`
  (params (bWasCancelled :type Boolean))
  (`KismetSystemLibrary.PrintString` (`KismetMathLibrary.SelectString` "Distract Cancelled" "Distract Ended" bWasCancelled)))

(fn `AOE Follow Stay`
  (locals (`L Found` :type "Array of Actor Object Reference") (`L Shouted Follow` :type Boolean) (`L Controller` :type "Controller Object Reference"))
  (bind _ascharacter (cast `Character` (`self.GetAvatarActorFromActorInfo`)))
  (set `local.L Controller` (`Pawn.GetController` _ascharacter))
  ;[1 1 1] When shouting beans, ai will follow or stay
  ; 1) Gather all AI in local area
  ; 2) If any are following you, stop all follows
  ; 3) If none are following you, request follow on any arrested perps with no leader, and any civilians who are rescued
  (bind _outactors (`KismetSystemLibrary.SphereOverlapActors` (`Actor.K2_GetActorLocation` (`self.GetAvatarActorFromActorInfo`)) 500.0 (`|MakeArray` "ObjectTypeQuery3" :!type "EObjectTypeQuery Enum") "/Game/Blueprints/Core/PolygonAI/BP_Polygon_AI.BP_Polygon_AI_C"))
  (set `local.L Found` _outactors)
  (`|ExecutionSequence`
    (:`then_0`
      ;[1 1 1] FOLLOW
      (for _array_element (`local.L Found`)
        (bind _asbp_polygon_ai_civilian (cast `/Game/Blueprints/Core/PolygonAI/BP_Polygon_AI_Civilian` _array_element)
          (:`then`
            (if (and (not (`KismetSystemLibrary.IsValid` (`/Game/Blueprints/Core/PolygonAI/BP_Polygon_AI.Leader` _asbp_polygon_ai_civilian))) (not (`/Game/Blueprints/Core/PolygonAI/BP_Polygon_AI.Arrested` _asbp_polygon_ai_civilian)) (not (`/Game/Blueprints/Core/PolygonAI/BP_Polygon_AI_Civilian.At APC` _asbp_polygon_ai_civilian)))
              (`/Game/Blueprints/Core/PolygonAI/BP_Polygon_AI.Set Following` _asbp_polygon_ai_civilian (`local.L Controller`) true)
              (set `local.L Shouted Follow` true :!label _label)))
          (:`CastFailed`
            (bind _asbp_polygon_ai (cast `/Game/Blueprints/Core/PolygonAI/BP_Polygon_AI` _array_element))
            (if (and (not (`KismetSystemLibrary.IsValid` (`/Game/Blueprints/Core/PolygonAI/BP_Polygon_AI.Leader` _asbp_polygon_ai))) (`/Game/Blueprints/Core/PolygonAI/BP_Polygon_AI.Arrested` _asbp_polygon_ai) (not (`/Game/Blueprints/Core/PolygonAI/BP_Polygon_AI_Civilian.At APC` _asbp_polygon_ai)))
              (`/Game/Blueprints/Core/PolygonAI/BP_Polygon_AI.Set Following` _asbp_polygon_ai (`local.L Controller`) true)
              (goto _label)))))
      ;[1 1 1] STOP
      (if (not (`local.L Shouted Follow`))
        (for _array_element_2 (`local.L Found`)
          (bind _asbp_polygon_ai_civilian_2 (cast `/Game/Blueprints/Core/PolygonAI/BP_Polygon_AI_Civilian` _array_element_2)
            (:`then`
              (if (and (== (`self.GetAvatarActorFromActorInfo`) (`/Game/Blueprints/Core/PolygonAI/BP_Polygon_AI.Leader` _asbp_polygon_ai_civilian_2)) (not (`/Game/Blueprints/Core/PolygonAI/BP_Polygon_AI.Arrested` _asbp_polygon_ai_civilian_2)) (not (`/Game/Blueprints/Core/PolygonAI/BP_Polygon_AI_Civilian.At APC` _asbp_polygon_ai_civilian_2)))
                (`/Game/Blueprints/Core/PolygonAI/BP_Polygon_AI.Set Following` _asbp_polygon_ai_civilian_2 (`local.L Controller`) false)))
            (:`CastFailed`
              (bind _asbp_polygon_ai_2 (cast `/Game/Blueprints/Core/PolygonAI/BP_Polygon_AI` _array_element_2))
              (if (and (`/Game/Blueprints/Core/PolygonAI/BP_Polygon_AI.Arrested` _asbp_polygon_ai_2) (== (`/Game/Blueprints/Core/PolygonAI/BP_Polygon_AI.Leader` _asbp_polygon_ai_2) (`self.GetAvatarActorFromActorInfo`)) (not (`/Game/Blueprints/Core/PolygonAI/BP_Polygon_AI_Civilian.At APC` _asbp_polygon_ai_2)))
                (`/Game/Blueprints/Core/PolygonAI/BP_Polygon_AI.Set Following` _asbp_polygon_ai_2 (`local.L Controller`) false)))))))))