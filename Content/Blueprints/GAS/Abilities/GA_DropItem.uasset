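; GA_DropItem is a Gameplay Ability that makes the character throw away an item from its inventory.
; It can activate only when BPInventoryComponent on the BP_Character_Template avatar returns a valid item.
; After committing, it plays the AM_ThrowWeapon montage at half speed, and the authority waits ThrowDelay before calling DropItem on that component.
; A failed commit cancels the ability, while the successful path never calls EndAbility.
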(event `self.K2_ActivateAbility`
  (`KismetSystemLibrary.PrintString` "On Activate Jump Ability" true true (struct :`R` 1.0 :`G` 0.406657 :`A` 1.0))
  (bind _returnvalue (`self.K2_CommitAbility`))
  (if _returnvalue
    (`GSCTask_PlayMontageWaitForEvent.PlayMontageAndWaitForEvent` "None" "/Game/Polygon/Animations/PolygonAnims/Warrior/AM_ThrowWeapon.AM_ThrowWeapon" (struct) 0.5 "None" false
      (:`then`
        (`self.K2_HasAuthority`
          (:`True`
            (`KismetSystemLibrary.Delay` (`self.Throw Delay`))
            (bind _asbp_character_template (cast `/Game/Blueprints/Core/BP_Character_Template` (`self.GetAvatarActorFromActorInfo`)))
            (`/Game/Blueprints/Items/BP_Inventory_Component.Drop Item` (`/Game/Blueprints/Core/BP_Character_Template.BP_Inventory_Component` _asbp_character_template) null)))))
    (else
      (`self.K2_CancelAbility`)
      (`KismetSystemLibrary.PrintString` "Cannot Commit Jump"))))

(fn `K2_CanActivateAbility`
  (params (ActorInfo :type "GameplayAbilityActorInfo Structure") (Handle :type "GameplayAbilitySpecHandle Structure"))
  (returns (RelevantTags :type "GameplayTagContainer Structure") (ReturnValue :type Boolean))
  (`|ExecutionSequence`
    (:`then_0`
      (bind _asbp_character_template (cast `/Game/Blueprints/Core/BP_Character_Template` (`self.GetAvatarActorFromActorInfo`)))
      (bind _item (`/Game/Blueprints/Items/BP_Inventory_Component.Get Items` (`/Game/Blueprints/Core/BP_Character_Template.BP_Inventory_Component` _asbp_character_template)))
      (`/Engine/EditorBlueprintResources/StandardMacros.IsValid` _item
        (:`Is Valid`
          (return (struct) true))))
    (:`then_1`
      (return (struct) false))))