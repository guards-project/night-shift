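; Gameplay ability that throws the avatar's equipped item, with separate player and AI paths and server-side throw logic.
; Players throw along their view on input release, with a long hold choosing the shield over the item.
; AI stops moving and launches on a montage event or interrupt, leading the cached target via suggested projectile velocity.
; AI then plays a rearm montage and, if empty-handed on end, clears throw abilities and equips a fresh copy.
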(event `self.K2_ActivateAbility`
  (`KismetSystemLibrary.PrintString` "Throw Ability" true true (struct :`R` 1.0 :`G` 0.406657 :`A` 1.0))
  (bind _returnvalue (`self.K2_CommitAbility`))
  (if _returnvalue
    (cast `/Game/Blueprints/Core/BP_Character_Template_Player` (`self.GetAvatarActorFromActorInfo`)
      (:`then`
        (set `self.is AI` false)
        (bind (_asynctaskproxy _timeheld) (`AbilityTask_WaitInputRelease.WaitInputRelease` false)
          (:`OnRelease`
            (set `self.Time Held` _timeheld)
            (`self.Start Throw`))))
      (:`CastFailed`
        (set `self.is AI` true)
        (`|ExecutionSequence`
          (:`then_0`
            (`self.K2_HasAuthority`
              (:`True`
                (`self.Set AI Movement Enabled` false))))
          (:`then_1`
            (`self.Start Throw`)
            (`AbilityAsync_WaitGameplayTagAdded.WaitGameplayTagAddToActor` (`self.GetAvatarActorFromActorInfo`) (struct :`TagName` "Status.Stunned") ; wait for a new combo tag\nonly once (after this attack started)
              (:`then`
                (`AbilityAsync_WaitGameplayTagAdded.WaitGameplayTagAddToActor` (`self.GetAvatarActorFromActorInfo`) (struct :`TagName` "Status.Dead") ; wait for a new combo tag\nonly once (after this attack started)
                  (:`Added`
                    (`self.K2_EndAbility`))))
              (:`Added`
                (`self.K2_EndAbility`)))))))
    (else
      (`KismetSystemLibrary.PrintString` (`KismetStringLibrary.Concat_StrStr` "THROW ERROR AI CANNOT COMMIT & WILL CANCEL"))
      (`self.K2_CancelAbility`)
      (`KismetSystemLibrary.PrintString` "Cannot Commit Throw" true true (struct :`G` 0.66 :`B` 1.0 :`A` 1.0) 10.0))))

(event `Start Throw`
  (if (`self.is AI`)
    ;[1 1 1] AI Throw
    (`KismetSystemLibrary.Delay` 0.7)
    (`GSCTask_PlayMontageWaitForEvent.PlayMontageAndWaitForEvent` "None" "/Game/Polygon/Animations/PolygonAnims/Carry/AM_ThrowOver.AM_ThrowOver" (struct :`GameplayTags` (struct :`(TagName` "Ability.Attack.Event"))) 0.5 "None" false
      (:`then`
        (`self.K2_HasAuthority`
          (:`True`
            (`|ExecutionSequence`
              (:`then_0`
                (`self.Set AI Movement Enabled` false)
                (bind _target (message `/Game/Blueprints/Core/PolygonAI/Behaviour/BPI_AI.Get Target` (`AIBlueprintHelperLibrary.GetAIController` (`self.GetAvatarActorFromActorInfo`))))
                (set `self.Cached Target` _target)
                (bind _item (message `/Game/Blueprints/Core/BPI_Character.Get Current Equipped Item` (`self.GetAvatarActorFromActorInfo`)))
                (bind _asbp_item (cast `/Game/Blueprints/Items/BP_Item` _item))
                (set `self.Item` _asbp_item))
              (:`then_1`
                (goto _label_2 :!via `Reset`))))))
      (:`OnInterrupted`
        (`KismetSystemLibrary.Delay` 0.5)
        (`self.K2_HasAuthority` :!label _label
          (:`True`
            (`/Engine/EditorBlueprintResources/StandardMacros.DoOnce` false :!label _label_2
              (:`Completed`
                (bind _item_2 (`self.Item`)
                  (:`then`
                    (set `self.Item to Spawn` (`GameplayStatics.GetObjectClass` _item_2))
                    (`self.Throw`)
                    (`self.AI Rearm Anim`))
                  (:`else`
                    (`self.K2_EndAbility`))))))))
      (:`EventReceived`
        (goto _label)))
    (else
      ;[1 1 1] Player Throw
      (`GSCTask_PlayMontageWaitForEvent.PlayMontageAndWaitForEvent` "None" "/Game/Polygon/Animations/PolygonAnims/Warrior/AM_ThrowWeapon.AM_ThrowWeapon" (struct) 0.5 "None" false
        (:`then`
          (`self.K2_HasAuthority`
            (:`True`
              (`KismetSystemLibrary.Delay` (`self.Throw Delay`))
              (bind _item_3 (message `/Game/Blueprints/Core/BPI_Character.Get Current Equipped Item` (`self.GetAvatarActorFromActorInfo`)))
              (`/Engine/EditorBlueprintResources/StandardMacros.IsValid` _item_3
                (:`Is Valid`
                  (`self.Throw`))
                (:`Is Not Valid`
                  (`self.K2_EndAbility`))))))))))

(event `Set AI Movement Enabled`
  (params (Enabled :type Boolean))
  (bind _asbp_polygon_ai (cast `/Game/Blueprints/Core/PolygonAI/BP_Polygon_AI` (`self.GetAvatarActorFromActorInfo`)))
  (`/Game/Blueprints/Core/BP_Character_Template.Auth Set Can Move` _asbp_polygon_ai Enabled))

(event `AI Rearm Anim`
  (bind _asbp_polygon_ai (cast `/Game/Blueprints/Core/PolygonAI/BP_Polygon_AI` (`self.GetAvatarActorFromActorInfo`))
    (:`then`
      (`self.Set AI Movement Enabled` false)
      (set `/Game/Blueprints/Core/PolygonAI/BP_Polygon_AI.Can Ever Telegraph Attack` false _asbp_polygon_ai)
      (`GSCTask_PlayMontageWaitForEvent.PlayMontageAndWaitForEvent` "None" "/Game/Polygon/Animations/PolygonAnims/Carry/AM_Polygon_Pickup2.AM_Polygon_Pickup2" (struct) 0.8 "None" false
        (:`then`
          (`KismetSystemLibrary.Delay` (`self.Throw Cooldown`))
          (`self.K2_EndAbility`))))
    (:`CastFailed`
      (`self.K2_EndAbility`))))

(event `self.K2_OnEndAbility`
  (params (bWasCancelled :type Boolean))
  (`parent.K2_OnEndAbility` bWasCancelled)
  (`self.K2_HasAuthority`
    (:`True`
      (if (`self.is AI`)
        (bind _item (message `/Game/Blueprints/Core/BPI_Character.Get Current Equipped Item` (`self.GetAvatarActorFromActorInfo`)))
        (`/Engine/EditorBlueprintResources/StandardMacros.IsValid` _item
          (:`Is Not Valid`
            (`self.AI Equip New Item`)))))))

(event `AI Equip New Item`
  (bind _returnvalue (`AbilitySystemBlueprintLibrary.GetAbilitySystemComponent` (`self.GetAvatarActorFromActorInfo`)))
  (bind _outabilityhandles (`AbilitySystemComponent.FindAllAbilitiesWithTags` _returnvalue (struct :`GameplayTags` (struct :`(TagName` "Ability.Throw"))) false))
  (for _array_element _outabilityhandles
    (`AbilitySystemComponent.ClearAbility` _returnvalue _array_element))
  (bind _item_to_spawn (`self.Item to Spawn`)
    (:`then`
      (bind _returnvalue_2 (`|SpawnActorFromClass` _item_to_spawn (`KismetMathLibrary.Conv_VectorToTransform` (0.0 0.0 0.0)) "AlwaysSpawn" "MultiplyWithRoot" null false null))
      (`/Game/Blueprints/Items/BP_Inventory_Component.Equip Item` (`Actor.GetComponentByClass` (`self.GetAvatarActorFromActorInfo`) "/Game/Blueprints/Items/BP_Inventory_Component.BP_Inventory_Component_C") _returnvalue_2))
    (:`else`)))

(fn `AI Throw`
  (returns (`Start Location` :type "Vector Structure") (`Prediction Velocity` :type "Vector Structure") (`AsBP Item` :type "/Game/Blueprints/Items/BP_Item Object Reference"))
  (locals (`L Item Location` :type "Vector Structure" :default (0.0 0.0 0.0)))
  (bind _cached_target (`self.Cached Target`)
    (:`then`
      (bind _item (`self.Item`)
        (:`then`
          (set `local.L Item Location` (`Actor.K2_GetActorLocation` _item))
          (bind _origin (`Actor.GetActorBounds` _cached_target true false))
          (bind (_tossvelocity _returnvalue) (`GameplayStatics.BlueprintSuggestProjectileVelocity` (`local.L Item Location`) (+ _origin (* (`Actor.GetVelocity` _cached_target) (/ (`KismetMathLibrary.Vector_Distance` (`local.L Item Location`) _origin) 2000.0))) 2000.0 0.0 "DoNotTrace" 10.0))
          (if _returnvalue
            (return (`local.L Item Location`) _tossvelocity (cast `/Game/Blueprints/Items/BP_Item` _item :!pure true))
            (else
              (return (0.0 0.0 0.0) (0.0 0.0 0.0) null))))
        (:`else`)))
    (:`else`
      (return (0.0 0.0 0.0) (0.0 0.0 0.0) null))))

(fn `K2_CanActivateAbility`
  (params (ActorInfo :type "GameplayAbilityActorInfo Structure") (Handle :type "GameplayAbilitySpecHandle Structure"))
  (returns (RelevantTags :type "GameplayTagContainer Structure") (ReturnValue :type Boolean))
  (`|ExecutionSequence`
    (:`then_0`
      (bind _asbp_character_template (cast `/Game/Blueprints/Core/BP_Character_Template` (`self.GetAvatarActorFromActorInfo`)))
      (bind (_item _shield) (`/Game/Blueprints/Items/BP_Inventory_Component.Get Items` (`/Game/Blueprints/Core/BP_Character_Template.BP_Inventory_Component` _asbp_character_template)))
      (return (struct) (or (`KismetSystemLibrary.IsValid` _item) (`KismetSystemLibrary.IsValid` _shield))))
    (:`then_1`
      (return (struct) false))))

(fn `Throw`
  (locals (`L Inventory` :type "/Game/Blueprints/Items/BP_Inventory_Component Object Reference") (`L Throw Item` :type "/Game/Blueprints/Items/BP_Item Object Reference") (`L Item` :type "/Game/Blueprints/Items/BP_Item Object Reference") (`L Shield` :type "/Game/Blueprints/Items/BP_Item Object Reference"))
  (bind _l_item (`local.L Item`))
  (bind _asbp_character_template (cast `/Game/Blueprints/Core/BP_Character_Template` (`self.GetAvatarActorFromActorInfo`)))
  (`/Engine/EditorBlueprintResources/StandardMacros.IsValid` (`AIBlueprintHelperLibrary.GetAIController` _asbp_character_template)
    (:`Is Valid`
      (bind (_start_location _prediction_velocity _asbp_item) (`self.AI Throw`))
      (`/Engine/EditorBlueprintResources/StandardMacros.IsValid` _asbp_item
        (:`Is Valid`
          (`/Game/Blueprints/Items/BP_Item.Throw Item` _asbp_item _start_location _prediction_velocity (0.0 5000.0 0.0) true) ; throw
        )))
    (:`Is Not Valid`
      (set `local.L Inventory` (`/Game/Blueprints/Core/BP_Character_Template.BP_Inventory_Component` _asbp_character_template))
      (bind (_item _shield) (`/Game/Blueprints/Items/BP_Inventory_Component.Get Items` (`local.L Inventory`)))
      (set `local.L Item` _item)
      (set `local.L Shield` _shield)
      (bind _output_get (set `local.L Throw Item` (select `bool` (> (`self.Time Held`) 0.5) :`false` (`local.L Item`) :`true` (`local.L Shield`))))
      (`/Engine/EditorBlueprintResources/StandardMacros.IsValid` _output_get
        (:`Is Valid`
          _)
        (:`Is Not Valid`
          ;[1 1 1] Fallback to either
          (bind _output_get_2 (set `local.L Throw Item` (select `bool` (`KismetSystemLibrary.IsValid` _l_item) :`false` (`local.L Shield`) :`true` _l_item)))
          (`/Engine/EditorBlueprintResources/StandardMacros.IsValid` _output_get_2
            (:`Is Valid`
              _))))
      (`/Game/Blueprints/Items/BP_Inventory_Component.Drop Item` (`local.L Inventory`) (`local.L Throw Item`))
      (bind _l_throw_item (`local.L Throw Item`)
        (:`then`
          (`/Game/Blueprints/Items/BP_Item.Throw Item` _l_throw_item (`Actor.GetActorEyesViewPoint` (`self.GetAvatarActorFromActorInfo`)) (* (`KismetMathLibrary.GetForwardVector` (`.OutRotation` (`Actor.GetActorEyesViewPoint` (`self.GetAvatarActorFromActorInfo`)))) 2000.0) (0.0 5000.0 0.0) true) ; throw
        )
        (:`else`
          _))
      (`self.K2_EndAbility`))))