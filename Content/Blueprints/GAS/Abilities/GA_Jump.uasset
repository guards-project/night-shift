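; GA_Jump is a Gameplay Ability that makes the avatar character jump with an animation.
; After committing, it starts the jump montage and immediately calls Jump and EndAbility, both only when the character is locally controlled.
; The montage task does not stop when the ability ends, so the animation continues.
; A failed commit cancels the ability and prints a debug message.
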(event `self.K2_ActivateAbility`
  (`KismetSystemLibrary.PrintString` "On Activate Jump Ability" true true (struct :`R` 1.0 :`G` 0.406657 :`A` 1.0))
  (bind _returnvalue (`self.K2_CommitAbility`))
  (if _returnvalue
    (`GSCTask_PlayMontageWaitForEvent.PlayMontageAndWaitForEvent` "None" "/Game/Polygon/Animations/PolygonAnims/Locomotion/AM_Polygon_Jump.AM_Polygon_Jump" (struct) 1.0 "None" false
      (:`then`
        (bind _ascharacter (cast `Character` (`self.GetAvatarActorFromActorInfo`)))
        (if (`Pawn.IsLocallyControlled` _ascharacter)
          (set `self.Character` _ascharacter)
          (`Character.Jump` (`self.Character`))
          (`self.K2_EndAbility`))))
    (else
      (`self.K2_CancelAbility`)
      (`KismetSystemLibrary.PrintString` "Cannot Commit Jump"))))