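; Gameplay ability, named as a guard Skol heal, that can activate only while the avatar's health is below maximum, as read from its BP_Health_Component.
; When the ability ends, whether cancelled or not, it runs the parent logic, then drops and destroys the avatar's currently equipped BP_Item.
; The healing itself is not implemented in these graphs.
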(event `self.K2_OnEndAbility`
  (params (bWasCancelled :type Boolean))
  (`parent.K2_OnEndAbility` bWasCancelled)
  (bind _item (message `/Game/Blueprints/Core/BPI_Character.Get Current Equipped Item` (`self.GetAvatarActorFromActorInfo`)))
  (`/Engine/EditorBlueprintResources/StandardMacros.IsValid` _item
    (:`Is Valid`
      (bind _asbp_item (cast `/Game/Blueprints/Items/BP_Item` _item))
      (`/Game/Blueprints/Items/BP_Item.Drop` _asbp_item)
      (`Actor.K2_DestroyActor` _asbp_item))))

(fn `K2_CanActivateAbility`
  (params (ActorInfo :type "GameplayAbilityActorInfo Structure") (Handle :type "GameplayAbilitySpecHandle Structure"))
  (returns (RelevantTags :type "GameplayTagContainer Structure") (ReturnValue :type Boolean))
  (bind _returnvalue (`Actor.GetComponentByClass` (`self.GetAvatarActorFromActorInfo`) "/Game/Blueprints/Core/Components/BP_Health_Component.BP_Health_Component_C"))
  (return (struct) (< (`/Game/Blueprints/Core/Components/BP_Health_Component.Get Health` _returnvalue) (`/Game/Blueprints/Core/Components/BP_Health_Component.Get Max Health` _returnvalue))))