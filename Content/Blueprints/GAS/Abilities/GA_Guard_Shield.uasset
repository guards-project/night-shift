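; GA_Guard_Shield is a Gameplay Ability for a shield guard that stays active while its input is held.
; On activation it commits, then uses a WaitInputRelease task to end the ability when the input is released, or cancels if the commit fails.
; It only manages the lifecycle with debug prints for activation, failed commit, end and cancel, and applies no shield effect in this graph.
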(event `self.K2_ActivateAbility`
  (`KismetSystemLibrary.PrintString` "On Activate Shield" true true (struct :`R` 1.0 :`G` 0.406657 :`A` 1.0))
  (bind _returnvalue (`self.K2_CommitAbility`))
  (if _returnvalue
    (`AbilityTask_WaitInputRelease.WaitInputRelease` true
      (:`OnRelease`
        (`self.K2_EndAbility`)))
    (else
      (`self.K2_CancelAbility`)
      (`KismetSystemLibrary.PrintString` "Cannot Commit Shield"))))

(event `self.K2_OnEndAbility`
  (params (bWasCancelled :type Boolean))
  (if bWasCancelled
    (`KismetSystemLibrary.PrintString` "Ability Cancelled: Shield")
    (else
      (`KismetSystemLibrary.PrintString` "Ability Ended: Shield"))))