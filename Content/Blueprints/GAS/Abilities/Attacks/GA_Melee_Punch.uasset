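; Melee punch Gameplay Ability that extends its parent's montage-driven attack with an optional fire projectile.
; A DoOnce, entered on montage events and re-armed when hit actors reset, limits the extra shot to once per reset.
; On authority, if the avatar has the Ability.Mod.FireAttacks tag, it spawns BP_Projectile_Fire just ahead of the eye viewpoint, with the avatar as owner and instigator.
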(event `self.Reset Hit Actors`
  (bind _returnvalue (`self.GetAvatarActorFromActorInfo`))
  (bind (_outlocation _outrotation) (`Actor.GetActorEyesViewPoint` _returnvalue))
  (`parent.Reset Hit Actors`)
  (goto _label :!via `Reset`))

(event `/Game/Blueprints/GAS/Abilities/Attacks/GA_UseItem_Master.Montage Event`
  (params (Tag :type "GameplayTag Structure") (Data :type "GameplayEventData Structure"))
  (bind _returnvalue (`self.GetAvatarActorFromActorInfo`))
  (bind (_outlocation _outrotation) (`Actor.GetActorEyesViewPoint` _returnvalue))
  (`parent.Montage Event` Tag Data)
  (`/Engine/EditorBlueprintResources/StandardMacros.DoOnce` false :!label _label
    (:`Completed`
      (`self.K2_HasAuthority`
        (:`True`
          (if (`GSCBlueprintFunctionLibrary.HasMatchingGameplayTag` _returnvalue (struct :`TagName` "Ability.Mod.FireAttacks"))
            (`|SpawnActorFromClass` "/Game/Blueprints/Items/Ranged/BP_Projectile_Fire.BP_Projectile_Fire_C" (`KismetMathLibrary.MakeTransform` (+ _outlocation (* (`KismetMathLibrary.Conv_RotatorToVector` _outrotation) 100.0)) _outrotation) "AdjustIfPossibleButAlwaysSpawn" "MultiplyWithRoot" _returnvalue (cast `Character` _returnvalue :!pure true))))))))