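; Melee attack gameplay ability for the lute that adds achievement reporting on top of its parent's attack behavior.
; It extends the parent's hit cue: when a locally controlled attack hits an actor tagged AI, it calls FryingPanJustice on the first player controller's achievement component.
; Activation and end events are disabled stubs, so the rest of the attack comes from the parent class.
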(event `self.Play Hit Cue`
  (params (Hit :type "HitResult Structure"))
  (bind (_bblockinghit _binitialoverlap _time _distance _location _impactpoint _normal _impactnormal _physmat _hitactor) (`GameplayStatics.BreakHitResult` Hit))
  (bind _returnvalue (`Actor.GetComponentByClass` (`GameplayStatics.GetPlayerController` 0) "/Game/_Guards/OnlineSubsystem/Achievements/BP_Achievement_Component.BP_Achievement_Component_C"))
  (`parent.Play Hit Cue` Hit)
  (`/Engine/EditorBlueprintResources/StandardMacros.IsValid` _hitactor
    (:`Is Valid`
      (if (`Actor.ActorHasTag` _hitactor "AI")
        (`self.IsLocallyControlled`
          (:`True`
            (`/Engine/EditorBlueprintResources/StandardMacros.IsValid` _returnvalue
              (:`Is Valid`
                (`/Game/_Guards/OnlineSubsystem/Achievements/BP_Achievement_Component.FryingPanJustice` _returnvalue)))))))))