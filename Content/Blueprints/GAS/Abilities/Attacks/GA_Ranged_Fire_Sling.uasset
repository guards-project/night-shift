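; Gameplay ability for firing a sling, which falls back to a blunt melee ability when it cannot activate.
; It overrides CanActivateAbility: if the parent check fails and the avatar is neither dead nor KO, it tries activating abilities tagged for equipped blunt melee on the avatar's ability system component.
; The parent's result and relevant tags return unchanged, so the fallback runs as a side effect of the activation check.
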(fn `K2_CanActivateAbility`
  (params (ActorInfo :type "GameplayAbilityActorInfo Structure") (Handle :type "GameplayAbilitySpecHandle Structure"))
  (returns (RelevantTags :type "GameplayTagContainer Structure") (ReturnValue :type Boolean))
  (bind (_owneractor _avataractor) (break `GameplayAbilityActorInfo` (`local.ActorInfo`)))
  (bind (_relevanttags _returnvalue) (`parent.K2_CanActivateAbility` ActorInfo Handle))
  (`|ExecutionSequence`
    (:`then_0`
      (if (not _returnvalue)
        (bind _dead (message `/Game/Blueprints/Core/BPI_Character.Is Dead` _avataractor))
        (bind _ko (message `/Game/Blueprints/Core/BPI_Character.Is KO` _avataractor))
        (if (not (or _dead _ko))
          (`AbilitySystemComponent.TryActivateAbilitiesByTag` (`GSCBlueprintFunctionLibrary.GetCompanionAbilitySystemComponent` _avataractor) (`BlueprintGameplayTagLibrary.MakeLiteralGameplayTagContainer` (struct :`GameplayTags` (struct :`(TagName` "Inventory.EquippedItem.Melee.Blunt")))) true))))
    (:`then_1`
      (return _relevanttags _returnvalue))))