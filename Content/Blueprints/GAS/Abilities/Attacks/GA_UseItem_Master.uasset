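; Base Gameplay Ability for using the equipped item, with montage-driven attack combos and empty hooks for child abilities.
; On commit it caches the item and plays a random or sequenced montage, advancing the index while the combo tag is present.
; Combo tag listeners manage an input window where player presses or delayed AI re-activation restart the use logic.
; Montage completion, a fallback timer, or server-detected Dead/KO tags end the ability.
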(event `self.K2_ActivateAbility`
  (bind _debug (`self.Debug`))
  (bind _debug_2 (`self.Debug`))
  (bind _debug_3 (`self.Debug`))
  (`self.End Ability On Downed`)
  (`KismetSystemLibrary.PrintString` "On Activate USE Ability" _debug _debug (struct :`R` 1.0 :`G` 0.406657 :`A` 1.0))
  (bind _returnvalue (`self.K2_CommitAbility`))
  (if _returnvalue
    (`KismetSystemLibrary.PrintString` "Commit USE" _debug_3 _debug_3)
    (bind _item (message `/Game/Blueprints/Core/BPI_Character.Get Current Equipped Item` (`self.GetAvatarActorFromActorInfo`)))
    (`/Engine/EditorBlueprintResources/StandardMacros.IsValid` _item
      (:`Is Valid`
        (bind _asbp_item (cast `/Game/Blueprints/Items/BP_Item` _item)
          (:`then`
            (`self.Cache Item` _asbp_item))
          (:`CastFailed`
            _)))
      (:`Is Not Valid`
        _))
    (`self.Start Use Logic`)
    (else
      (`self.K2_CancelAbility`)
      (`KismetSystemLibrary.PrintString` "Cannot Commit USE" _debug_2 _debug_2))))

(event `Start Use Logic`
  (bind _debug (`self.Debug`))
  (`self.Debug Use Count`)
  (set `self.Active` true)
  (bind (_asynctaskproxy _eventtag _eventdata) (`GSCTask_PlayMontageWaitForEvent.PlayMontageAndWaitForEvent` "None" (`self.Get Combo Montage`) (`self.Montage Event Tag`) 1.0 "None" false)
    (:`then`
      (`self.Init Fallback End`)
      ;[1 1 1] Combo Tag Bindings
      (if (`BlueprintGameplayTagLibrary.IsGameplayTagValid` (`self.Combo Tag`))
        (`KismetSystemLibrary.PrintString` (`KismetStringLibrary.Concat_StrStr` "Combo Index: " (`KismetStringLibrary.Conv_IntToString` (`self.Combo Index`))) _debug _debug)
        (`self.Unbind All Events`)
        (`AbilitySystemBlueprintLibrary.RemoveLooseGameplayTags` (`self.GetAvatarActorFromActorInfo`) (`BlueprintGameplayTagLibrary.MakeGameplayTagContainerFromArray` (`|MakeArray` (`self.Combo Tag`)))) ; remove any existing combo tags from the player
        (bind _asynctaskproxy_2 (`AbilityAsync_WaitGameplayTagAdded.WaitGameplayTagAddToActor` (`self.GetAvatarActorFromActorInfo`) (`self.Combo Tag`) true) ; wait for a new combo tag\nonly once (after this attack started)
          (:`then`
            (bind _output_get (set `self.Async Action Add Combo Tag` _asynctaskproxy_2))
            (add `AbilityAsync_WaitGameplayTagAdded.Added` _output_get (`|CreateDelegate` :!event `Combo Open`)) ; bind to tag added
          ))))
    (:`OnCompleted`
      (`self.Montage Complete`))
    (:`OnBlendOut`
      (`self.Montage Blend Out`))
    (:`OnInterrupted`
      (`self.Montage Interrupted`))
    (:`OnCancelled`
      (`self.Montage Cancelled`))
    (:`EventReceived`
      (`self.Montage Event` _eventtag _eventdata))))

(event `Montage Complete`
  (`self.K2_EndAbility`))

(event `Montage Interrupted`)

(event `Montage Cancelled`)

(event `Montage Blend Out`)

(event `Montage Event`
  (params (Tag :type "GameplayTag Structure") (Data :type "GameplayEventData Structure")))

(event `Stop Use Logic`)

(event `Combo Open`
  (bind _debug (`self.Debug`))
  ;[1 1 1] Combo Tag Bindings
  (`KismetSystemLibrary.PrintString` (`KismetStringLibrary.Concat_StrStr` "Combo Window Open " (`KismetSystemLibrary.GetDisplayName` self)) _debug _debug (struct :`G` 0.729167 :`B` 0.076322 :`A` 1.0))
  (`|ExecutionSequence`
    (:`then_0`
      (if (and (`Actor.ActorHasTag` (`self.GetAvatarActorFromActorInfo`) "AI") (`self.Can AI Combo`))
        (`KismetSystemLibrary.Delay` (`self.Get Combo Delay`))
        (`AbilitySystemComponent.TryActivateAbilitiesByTag` (`AbilitySystemBlueprintLibrary.GetAbilitySystemComponent` (`self.GetAvatarActorFromActorInfo`)) (`BlueprintGameplayTagLibrary.MakeLiteralGameplayTagContainer` (struct :`GameplayTags` (struct :`(TagName` "Inventory.EquippedItem")))) true)))
    (:`then_1`
      (bind _asynctaskproxy (`AbilityTask_WaitAbilityActivate.WaitForAbilityActivate` (struct :`TagName` "Inventory.EquippedItem") (struct) true) ; AI\ndoesn't work on player for some reason\nSee end of this line for player input
        (:`then`
          (bind _output_get (set `self.Async Ability Activated` _asynctaskproxy))
          (add `AbilityTask_WaitAbilityActivate.OnActivate` _output_get (delegate `On Ability Activated`))
          (bind _asynctaskproxy_2 (`AbilityAsync_WaitGameplayTagRemoved.WaitGameplayTagRemoveFromActor` (`self.GetAvatarActorFromActorInfo`) (`self.Combo Tag`))
            (:`then`
              (bind _output_get_2 (set `self.Async Action Remove Combo Tag` _asynctaskproxy_2))
              (add `AbilityAsync_WaitGameplayTagRemoved.Removed` _output_get_2 (`|CreateDelegate` :!event `Combo Closed`))
              ;;[1 1 1] Player Input
              (bind _asynctaskproxy_3 (`AbilityTask_WaitInputPress.WaitInputPress` false) ; when the window is opened, wait for input
                (:`then`
                  (bind _output_get_3 (set `self.Async Wait Input` _asynctaskproxy_3))
                  (`/Engine/EditorBlueprintResources/StandardMacros.IsValid` _output_get_3
                    (:`Is Valid`
                      (add `AbilityTask_WaitInputPress.OnPress` _output_get_3 (delegate `On Press during Combo Window`)))))))))))))

(event `self.K2_OnEndAbility`
  (params (bWasCancelled :type Boolean))
  (bind _debug (`self.Debug`))
  (set `self.Active` false)
  (`KismetSystemLibrary.PrintString` "Ability Ended: Use" _debug _debug)
  (`self.Stop Use Logic`)
  (`self.Unbind All Events`))

(event `On Press during Combo Window`
  (params (TimeWaited :type "Float (single-precision)"))
  (bind _debug (`self.Debug`))
  ;[1 1 1] Combo Tag Bindings
  ;;[1 1 1] Player Input
  (`KismetSystemLibrary.PrintString` (`KismetStringLibrary.Concat_StrStr` "Input Pressed during Combo Window" (`KismetSystemLibrary.GetDisplayName` self)) _debug _debug (struct :`G` 0.729167 :`B` 0.076322 :`A` 1.0))
  (`self.Start Use Logic`))

(event `On Ability Activated`
  (params (ActivatedAbility :type "GameplayAbility Object Reference"))
  (bind _debug (`self.Debug`))
  ;[1 1 1] Combo Tag Bindings
  (if (== ActivatedAbility self)
    (`KismetSystemLibrary.PrintString` (`KismetStringLibrary.Concat_StrStr` "Input Pressed during Combo Window" (`KismetSystemLibrary.GetDisplayName` self)) _debug _debug (struct :`G` 0.729167 :`B` 0.076322 :`A` 1.0))
    (`self.Start Use Logic`)))

(event `Combo Closed`
  ;[1 1 1] Combo Tag Bindings
  (`self.K2_EndAbility`))

(event `Init Fallback End`
  (bind _fallback_duration (`self.Fallback Duration`))
  (if (> _fallback_duration 0.0)
    (bind _returnvalue (`KismetSystemLibrary.K2_SetTimerDelegate` (delegate `Fallback End`) _fallback_duration))
    (set `self.Fallback End Timer` _returnvalue)))

(event `Unbind All Events`
  ;[1 1 1] Combo Tag Bindings
  (`|ExecutionSequence`
    (:`then_0`
      (bind _async_action_remove_combo_tag (`self.Async Action Remove Combo Tag`)
        (:`then`
          (remove `AbilityAsync_WaitGameplayTagRemoved.Removed` _async_action_remove_combo_tag (`|CreateDelegate` :!event `Combo Closed`)))
        (:`else`)))
    (:`then_1`
      (bind _async_action_add_combo_tag (`self.Async Action Add Combo Tag`)
        (:`then`
          (remove `AbilityAsync_WaitGameplayTagAdded.Added` _async_action_add_combo_tag (`|CreateDelegate` :!event `Combo Open`)))
        (:`else`)))
    (:`then_2`
      (bind _async_ability_activated (`self.Async Ability Activated`)
        (:`then`
          (remove `AbilityTask_WaitAbilityActivate.OnActivate` _async_ability_activated (`|CreateDelegate` :!event `On Ability Activated`)))
        (:`else`)))
    (:`then_3`
      (bind _async_wait_input (`self.Async Wait Input`)
        (:`then`
          (remove `AbilityTask_WaitInputPress.OnPress` _async_wait_input (`|CreateDelegate` :!event `On Press during Combo Window`)))
        (:`else`)))))

(event `Fallback End`
  (`self.K2_EndAbility`))

(event `End Ability On Downed`
  (`self.K2_HasAuthority`
    (:`True`
      (bind _asynctaskproxy (`AbilityTask_WaitGameplayTagAdded.WaitGameplayTagAdd` (struct :`TagName` "Status.Dead") (`self.GetAvatarActorFromActorInfo`))
        (:`then`
          (bind _output_get (set `self.Dead` _asynctaskproxy))
          (add `AbilityTask_WaitGameplayTagAdded.Added` _output_get (delegate `On Dead`))
          (bind _asynctaskproxy_2 (`AbilityTask_WaitGameplayTagAdded.WaitGameplayTagAdd` (struct :`TagName` "Status.KO") (`self.GetAvatarActorFromActorInfo`))
            (:`then`
              (bind _output_get_2 (set `self.KO` _asynctaskproxy_2))
              (add `AbilityTask_WaitGameplayTagAdded.Added` _output_get_2 (delegate `On KO`)))))))))

(event `On Dead`
  (`self.K2_EndAbility`))

(event `On KO`
  (`self.K2_EndAbility`))

(fn `Cache Item`
  (params (Item :type "/Game/Blueprints/Items/BP_Item Object Reference"))
  (set `self.Item` Item))

(fn `Debug Use Count`
  (bind _debug (`self.Debug`))
  (`KismetSystemLibrary.PrintString` (`KismetStringLibrary.Concat_StrStr` "Start Use Logic " (`KismetSystemLibrary.GetDisplayName` self) " uses: " (`KismetStringLibrary.Conv_IntToString` (`self.Uses`))) _debug _debug (struct :`G` 0.729167 :`B` 0.076322 :`A` 1.0))
  (`/Engine/EditorBlueprintResources/StandardMacros.IncrementInt` (`self.Uses`)))

(fn `Get Combo Delay`
  (returns (ReturnValue :type "Float (double-precision)"))
  (bind _item (`self.Item`)
    (:`then`
      (bind (_ai_combo_delay_range_x _ai_combo_delay_range_y) (`KismetMathLibrary.BreakVector2D` (`/Game/Blueprints/Items/BP_Item.AI Combo Delay Range` _item)))
      (return (`KismetMathLibrary.RandomFloatInRange` _ai_combo_delay_range_x _ai_combo_delay_range_y)))
    (:`else`
      (return (`KismetMathLibrary.RandomFloatInRange` 0.1 0.2)))))

(fn `Get Combo Montage`
  (returns (OutItem :type "AnimMontage Object Reference"))
  (bind _returnvalue (+ (`self.Combo Index`) 1))
  (if (`self.Montage Sequence`)
    (if (`GameplayTagAssetInterface.HasMatchingGameplayTag` (`AbilitySystemBlueprintLibrary.GetAbilitySystemComponent` (`self.GetAvatarActorFromActorInfo`)) (struct :`TagName` "Ability.Attack.Combo"))
      (set `self.Combo Index` (`KismetMathLibrary.SelectInt` 0 _returnvalue (== _returnvalue (`KismetArrayLibrary.Array_Length` (`self.Montages`)))))
      (`|ExecutionSequence`
        (:`then_0`
          (if (== (`self.Combo Index`) 0)
            (bind _item (`self.Item`)
              (:`then`
                (set `/Game/Blueprints/Items/BP_Item.Combo Complete` true _item))
              (:`else`))))
        (:`then_1`
          (bind _output_get (set `self.Current Montage` (`|GetArrayItem` (`self.Montages`) (`self.Combo Index`))))
          (return _output_get)))
      (else
        (`|ExecutionSequence`
          (:`then_0`
            ;[1 1 1] no combo window & combo index was more than 0 means its the last combo in a sequence
            (if (!= (`self.Combo Index`) 0)
              (bind _item_2 (`self.Item`)
                (:`then`
                  (set `/Game/Blueprints/Items/BP_Item.Combo Complete` true _item_2)
                  (set `self.Active` false))
                (:`else`))))
          (:`then_1`
            (set `self.Combo Index` 0)
            (set `self.Current Montage` (`|GetArrayItem` (`self.Montages`)))
            (return (`self.Current Montage`))))))
    (else
      (return (`KismetArrayLibrary.Array_Random` (`self.Montages`))))))