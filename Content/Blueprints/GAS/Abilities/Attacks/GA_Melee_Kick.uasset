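; Melee kick gameplay ability that damages and stuns what it hits, launching ragdolled characters forward and up for fun.
; Extends a parent attack ability, firing its montage event after a short delay on start.
; Hits come from a multi-object sphere trace below eye level along the view direction, ignoring already-hit actors; box-trace alternatives are left unused.
; Damage handling calls the parent, then adds a death impulse at the hit bone and an AOE stun for character targets.
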(event `/Game/Blueprints/GAS/Abilities/Attacks/GA_UseItem_Master.Start Use Logic`
  (`parent.Start Use Logic`)
  (`KismetSystemLibrary.Delay` 0.3)
  (`parent.Montage Event` (struct) (struct)))

(fn `Gather Hits`
  (bind _returnvalue (`self.GetAvatarActorFromActorInfo`))
  (bind (_outlocation _outrotation) (`Actor.GetActorEyesViewPoint` _returnvalue))
  (bind _returnvalue_2 (+ (- _outlocation (0.0 0.0 50.0)) (* (`Actor.GetActorForwardVector` _returnvalue) (`self.Default Trace Start Offset`))))
  ;[1 1 1] Rectangle
  (bind _outhits (`KismetSystemLibrary.SphereTraceMultiForObjects` _returnvalue_2 (+ _returnvalue_2 (* (`KismetMathLibrary.GetForwardVector` _outrotation) (`self.Trace Length`))) (`self.Trace Radius`) (`|MakeArray` "ObjectTypeQuery1" "ObjectTypeQuery2" "ObjectTypeQuery3" "ObjectTypeQuery4" "ObjectTypeQuery7" "ObjectTypeQuery8" :!type "EObjectTypeQuery Enum") false (`self.Get Ignored Actors`) (`self.Debug Type`)))
  (`self.Cache Valid Hits` _outhits)
  (return))

(fn `Get Damage`
  (returns (Damage :type "Float (single-precision)"))
  (return (`self.Default Damage`)))

(fn `Get Damage Type`
  (returns (`Damage Type` :type "DamageType Class Reference"))
  (return (`self.Default Damage Type`)))

(fn `Get Ignored Actors`
  (returns (Array :type "Array of Actor Object Reference"))
  (locals (`L Array` :type "Array of Actor Object Reference"))
  (bind _output_get (set `local.L Array` (`parent.Get Ignored Actors`)))
  (`KismetArrayLibrary.Array_Append` _output_get (`self.Already Hit Actors`))
  (return (`local.L Array`)))

(fn `Handle Damage Event`
  (params (Hit :type "HitResult Structure (by ref)"))
  (bind (_bblockinghit _binitialoverlap _time _distance _location _impactpoint _normal _impactnormal _physmat _hitactor _hitcomponent _hitbonename) (`GameplayStatics.BreakHitResult` Hit))
  (`parent.Handle Damage Event` Hit)
  (bind _asbp_character_template (cast `/Game/Blueprints/Core/BP_Character_Template` _hitactor))
  (`/Game/Blueprints/Core/BP_Character_Template.MC Death Impulse` _asbp_character_template (+ (* (`Actor.GetActorForwardVector` (`self.GetAvatarActorFromActorInfo`)) 20000.0) (0.0 0.0 10000.0)) _hitbonename) ; if ragdolled from kick\nadd a big impulse \nfor fun
  (`self.AOE Stun` (`local.Hit`))
  (return))