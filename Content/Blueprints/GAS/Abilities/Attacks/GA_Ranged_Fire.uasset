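; GA_Ranged_Fire is a gameplay ability that fires the equipped ranged weapon while input is held.
; Activation requires the State.Aiming tag or an AI avatar, plus an inactive shoot timer, and bypasses the parent's check.
; On authority, it starts firing on the cached weapon if able.
; Input release or the weapon's stopped-firing event ends the ability, which stops any ongoing fire.
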(event `self.K2_ActivateAbility`
  (`parent.K2_ActivateAbility`)
  (`AbilityTask_WaitInputRelease.WaitInputRelease` true
    (:`then`
      (`self.Fire`))
    (:`OnRelease`
      ;[1 0 0] !!!! TIL This fires instantly if the IA_Input is not set to 'down' !!!!
      (`self.K2_EndAbility`) ; !!!! This fires instantly if the IA_Input is not set to 'down' !!!!
    )))

(event `self.K2_OnEndAbility`
  (params (bWasCancelled :type Boolean))
  (`parent.K2_OnEndAbility` bWasCancelled)
  (bind _ranged_weapon (`self.Ranged Weapon`)
    (:`then`
      (if (`/Game/Blueprints/Items/Ranged/BP_Item_RangedWeapon.Is Firing` _ranged_weapon)
        (`/Game/Blueprints/Items/Ranged/BP_Item_RangedWeapon.Stop Firing` (`self.Ranged Weapon`))))
    (:`else`)))

(event `Fire`
  (bind _ranged_weapon (`self.Ranged Weapon`))
  (`self.K2_HasAuthority`
    (:`True`
      (if (and (`/Game/Blueprints/Items/Ranged/BP_Item_RangedWeapon.Can Fire` _ranged_weapon) (not (`/Game/Blueprints/Items/Ranged/BP_Item_RangedWeapon.Is Firing` _ranged_weapon)))
        (`/Game/Blueprints/Items/Ranged/BP_Item_RangedWeapon.Start Firing` _ranged_weapon)))))

(event `OnFiringStateChanged`
  (params (`Is Firing` :type Boolean))
  (if (not `Is Firing`)
    (`self.K2_EndAbility`)))

(fn `Cache Item`
  (params (Item :type "/Game/Blueprints/Items/BP_Item Object Reference"))
  (`parent.Cache Item` Item)
  (bind _asbp_item_ranged_weapon (cast `/Game/Blueprints/Items/Ranged/BP_Item_RangedWeapon` Item))
  (bind _output_get (set `self.Ranged Weapon` _asbp_item_ranged_weapon))
  (add `/Game/Blueprints/Items/Ranged/BP_Item_RangedWeapon.Firing State Changed` _output_get (`|CreateDelegate` :!event `OnFiringStateChanged`)))

(fn `K2_CanActivateAbility`
  (params (ActorInfo :type "GameplayAbilityActorInfo Structure") (Handle :type "GameplayAbilitySpecHandle Structure"))
  (returns (RelevantTags :type "GameplayTagContainer Structure") (ReturnValue :type Boolean))
  (bind (_owneractor _avataractor) (break `GameplayAbilityActorInfo` ActorInfo))
  (bind _item (message `/Game/Blueprints/Core/BPI_Character.Get Current Equipped Item` _avataractor))
  (return (struct) (and true (or (`GSCBlueprintFunctionLibrary.HasMatchingGameplayTag` _avataractor (struct :`TagName` "State.Aiming")) (`.bSuccess` (cast `/Game/Blueprints/Core/PolygonAI/BP_Polygon_AI` _avataractor :!pure true))) (not (`KismetSystemLibrary.K2_IsTimerActiveHandle` (`/Game/Blueprints/Items/Ranged/BP_Item_RangedWeapon.Shoot Timer` (cast `/Game/Blueprints/Items/Ranged/BP_Item_RangedWeapon` _item :!pure true)))))))