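; GA_Melee_Spin is a melee spin attack ability that builds on its parent's use logic and repeats while the same melee item stays equipped.
; Locally controlled characters switch to third-person camera, with the previous view restored on end, and non-AI avatars end the ability upon guarding.
; AI restarts the attack when stun is removed or its target changes.
; Each use clears Active after a short delay.
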(event `self.K2_ActivateAbility`
  (bind _returnvalue (`self.GetAvatarActorFromActorInfo`))
  (`parent.K2_ActivateAbility`)
  (`|ExecutionSequence`
    (:`then_0`
      (bind _guards_character (`self.Guards Character`)
        (:`then`
          (if (`Pawn.IsLocallyControlled` _guards_character)
            (bind _was_third (message `/Game/Blueprints/Core/BPI_Character.Set 3P Camera` (`self.GetAvatarActorFromActorInfo`) true))
            (set `self.Was Third` _was_third)))
        (:`else`)))
    (:`then_1`
      (if (`Actor.ActorHasTag` _returnvalue "AI")
        (bind _asynctaskproxy (`AbilityAsync_WaitGameplayTagRemoved.WaitGameplayTagRemoveFromActor` _returnvalue (struct :`TagName` "Status.Stunned"))
          (:`then`
            (bind _output_get (set `self.Removed` _asynctaskproxy))
            (add `AbilityAsync_WaitGameplayTagRemoved.Removed` _output_get (delegate `On Removed Stun`))
            (bind _asai_controller_polygon (cast `/Game/Blueprints/Core/PolygonAI/Behaviour/AI_Controller_Polygon` (`AIBlueprintHelperLibrary.GetAIController` (`self.GetAvatarActorFromActorInfo`))))
            (add `/Game/Blueprints/Core/PolygonAI/Behaviour/AI_Controller_Polygon.Target Changed` _asai_controller_polygon (delegate `Target Changed_Event`))))
        (else
          (`AbilityAsync_WaitGameplayTagAdded.WaitGameplayTagAddToActor` (`self.GetAvatarActorFromActorInfo`) (struct :`TagName` "State.Guarding")
            (:`Added`
              (`self.K2_EndAbility`))))))))

(event `self.K2_OnEndAbility`
  (params (bWasCancelled :type Boolean))
  (`parent.K2_OnEndAbility` bWasCancelled)
  (message `/Game/Blueprints/Core/BPI_Character.Set 3P Camera` (`self.GetAvatarActorFromActorInfo`) (`self.Was Third`)))

(event `On Removed Stun`
  (`self.Start Use Logic`))

(event `Target Changed_Event`
  (params (Controller :type "/Game/Blueprints/Core/PolygonAI/Behaviour/AI_Controller_Polygon Object Reference"))
  (`self.Start Use Logic`))

(event `self.Montage Complete`
  (bind _item (message `/Game/Blueprints/Core/BPI_Character.Get Current Equipped Item` (`self.GetAvatarActorFromActorInfo`) :!label _label))
  (`/Engine/EditorBlueprintResources/StandardMacros.IsValid` _item
    (:`Is Valid`
      (if (== _item (`self.Melee Item`))
        (`self.Start Use Logic`)))))

(event `self.Montage Blend Out`
  (goto _label))

(event `self.Fallback End`
  (goto _label))

(event `self.Start Use Logic`
  (`parent.Start Use Logic`)
  (`KismetSystemLibrary.Delay` 1.0)
  (set `self.Active` false))