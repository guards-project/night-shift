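; Gameplay ability for the exploder variant of the torch melee attack, turning a hit into an explosion.
; It handles the ApplyDamage event by dealing radial damage around the hit location with an insta-kill lethal damage type, credited to the avatar's instigator controller.
; A non-player avatar is excluded from its own blast, while one tagged Player is not ignored and can be caught in it.
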(event `self.Apply Damage`
  (params (Hit :type "HitResult Structure (by ref)"))
  (bind _returnvalue (`self.GetAvatarActorFromActorInfo`))
  (`GameplayStatics.ApplyRadialDamage` 50.0 (`.Location` (`GameplayStatics.BreakHitResult` Hit)) 800.0 "/Game/Blueprints/Items/DamageTypes/DamageType_Polygon_Lethal_InstaKill.DamageType_Polygon_Lethal_InstaKill_C" (select `bool` (`Actor.ActorHasTag` _returnvalue "Player") :`false` (`|MakeArray` _returnvalue) :`true` (`|MakeArray` null :!type "Actor Object Reference")) (`self.Get Damage Causer`) (`Pawn.GetController` (`Actor.Instigator` (`self.GetAvatarActorFromActorInfo`)))))