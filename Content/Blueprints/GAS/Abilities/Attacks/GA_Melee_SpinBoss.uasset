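; GA_Melee_SpinBoss is a melee spin attack ability, named for a boss, that knocks hit characters away and stuns them.
; It extends the parent's ApplyDamage, then launches any hit BP_Character_Template outward from the attacker with a slight lift, overriding its velocity.
; The stun is deferred via a one-shot landed-event binding, which unbinds and applies GE_Stun_1s through the victim's ability system component.
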(event `/Game/Blueprints/GAS/Abilities/Attacks/GA_Melee.Apply Damage`
  (params (Hit :type "HitResult Structure (by ref)"))
  (bind (_bblockinghit _binitialoverlap _time _distance _location _impactpoint _normal _impactnormal _physmat _hitactor) (`GameplayStatics.BreakHitResult` Hit))
  (bind (_returnvalue_x _returnvalue_y) (`KismetMathLibrary.BreakVector` (* (`KismetMathLibrary.GetDirectionUnitVector` (`Actor.K2_GetActorLocation` (`self.GetAvatarActorFromActorInfo`)) (`Actor.K2_GetActorLocation` _hitactor)) 2.0)))
  (`parent.Apply Damage` Hit)
  (bind _asbp_character_template (cast `/Game/Blueprints/Core/BP_Character_Template` _hitactor))
  (`Character.LaunchCharacter` _asbp_character_template (* (`KismetMathLibrary.MakeVector` _returnvalue_x _returnvalue_y 0.4) 750.0) true true)
  (add `/Game/Blueprints/Core/BP_Character_Template.Character Landed` _asbp_character_template (delegate `Character Landed_Event`)))

(event `Character Landed_Event`
  (params (Character :type "/Game/Blueprints/Core/BP_Character_Template Object Reference"))
  (remove `/Game/Blueprints/Core/BP_Character_Template.Character Landed` Character (delegate `Character Landed_Event`))
  (`AbilitySystemComponent.BP_ApplyGameplayEffectToSelf` :`self` (`AbilitySystemBlueprintLibrary.GetAbilitySystemComponent` Character) :`GameplayEffectClass` "/Game/Blueprints/GAS/Effects/GE_Stun_1s.GE_Stun_1s_C"))