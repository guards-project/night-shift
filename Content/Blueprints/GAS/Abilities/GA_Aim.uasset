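; GA_Aim is a Gameplay Ability that handles hold-to-aim for the player character.
; Activation commits the ability, or cancels it on failure, then waits for input release to end it.
; On authority only, it switches BP_Character_Template_Player's move state through AuthSetMoveState while active and sets a second state whenever the ability ends or is cancelled.
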(event `self.K2_ActivateAbility`
  (bind _debug (`self.Debug`))
  (bind _debug_2 (`self.Debug`))
  (`KismetSystemLibrary.PrintString` "On Activate Aim Ability" _debug_2 _debug_2 (struct :`R` 1.0 :`G` 0.406657 :`A` 1.0))
  (bind _returnvalue (`self.K2_CommitAbility`))
  (if _returnvalue
    (`AbilityTask_WaitInputRelease.WaitInputRelease` true
      (:`then`
        (`self.K2_HasAuthority`
          (:`True`
            (bind _asbp_character_template_player (cast `/Game/Blueprints/Core/BP_Character_Template_Player` (`self.GetAvatarActorFromActorInfo`)))
            (`/Game/Blueprints/Core/BP_Character_Template.Auth Set Move State` _asbp_character_template_player "NewEnumerator0"))))
      (:`OnRelease`
        (`self.K2_EndAbility`)))
    (else
      (`self.K2_CancelAbility`)
      (`KismetSystemLibrary.PrintString` "Cannot Commit Aim" _debug _debug))))

(event `self.K2_OnEndAbility`
  (params (bWasCancelled :type Boolean))
  (bind _debug (`self.Debug`))
  (if bWasCancelled
    (`KismetSystemLibrary.PrintString` "Ability Cancelled: Aim" _debug _debug)
    (else
      (`KismetSystemLibrary.PrintString` "Ability Ended: Aim" _debug _debug)))
  (`self.K2_HasAuthority`
    (:`True`
      (bind _asbp_character_template_player (cast `/Game/Blueprints/Core/BP_Character_Template_Player` (`self.GetAvatarActorFromActorInfo`)))
      (`/Game/Blueprints/Core/BP_Character_Template.Auth Set Move State` _asbp_character_template_player "NewEnumerator1"))))