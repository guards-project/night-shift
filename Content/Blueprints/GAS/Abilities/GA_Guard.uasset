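; GA_Guard is a Gameplay Ability for a guard action that stays active while its input is held.
; On activation it commits the ability, then waits for input release to end itself; a failed commit cancels it.
; The graph itself only manages this lifecycle, with debug prints for activation, commit failure, cancellation and normal end.
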(event `self.K2_ActivateAbility`
  (bind _debug (`self.Debug`))
  (bind _debug_2 (`self.Debug`))
  (`KismetSystemLibrary.PrintString` "On Activate Guard Ability" _debug _debug (struct :`R` 1.0 :`G` 0.406657 :`A` 1.0))
  (bind _returnvalue (`self.K2_CommitAbility`))
  (if _returnvalue
    (`AbilityTask_WaitInputRelease.WaitInputRelease` true
      (:`OnRelease`
        (`self.K2_EndAbility`)))
    (else
      (`self.K2_CancelAbility`)
      (`KismetSystemLibrary.PrintString` "Cannot Commit Guard" _debug_2 _debug_2))))

(event `self.K2_OnEndAbility`
  (params (bWasCancelled :type Boolean))
  (bind _debug (`self.Debug`))
  (if bWasCancelled
    (`KismetSystemLibrary.PrintString` "Ability Cancelled: Guard" _debug _debug)
    (else
      (`KismetSystemLibrary.PrintString` "Ability Ended: Guard" _debug _debug))))