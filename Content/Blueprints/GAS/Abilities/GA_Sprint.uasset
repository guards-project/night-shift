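; GAS sprint ability for the template character, allowed only when its velocity direction roughly matches its facing.
; On commit, the authority sets the move state and applies GE_Sprint, while the locally controlled side uncrouches.
; The Input.HoldSprint CVar decides whether input release or a second press ends it.
; On end, the authority restores the move state and removes the effect only if the state is still unchanged.
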(event `self.K2_ActivateAbility`
  (`KismetSystemLibrary.PrintString` "On Activate Sprint Ability" true true (struct :`R` 1.0 :`G` 0.406657 :`A` 1.0))
  (bind _returnvalue (`self.K2_CommitAbility`))
  (if _returnvalue
    (`|ExecutionSequence`
      (:`then_0`
        (`self.K2_HasAuthority`
          (:`True`
            (bind _asbp_character_template (cast `/Game/Blueprints/Core/BP_Character_Template` (`self.GetAvatarActorFromActorInfo`)))
            (`/Game/Blueprints/Core/BP_Character_Template.Auth Set Move State` _asbp_character_template "NewEnumerator2")
            (bind _returnvalue_2 (`self.BP_ApplyGameplayEffectToOwner` "/Game/Blueprints/GAS/Effects/GE_Sprint.GE_Sprint_C"))
            (set `self.EffectHandle` _returnvalue_2))))
      (:`then_1`
        (`self.IsLocallyControlled`
          (:`True`
            (bind _asbp_character_template_2 (cast `/Game/Blueprints/Core/BP_Character_Template` (`self.GetAvatarActorFromActorInfo`)))
            (`Character.UnCrouch` _asbp_character_template_2)
            (if (`ConsoleUtils.GetBoolCVar` "Input.HoldSprint")
              (`AbilityTask_WaitInputRelease.WaitInputRelease` true ; end when hoild released
                (:`OnRelease`
                  (`self.K2_EndAbility`)))
              (else
                (`AbilityTask_WaitInputPress.WaitInputPress` false ; end when the button is pressed again
                  (:`OnPress`
                    (`self.K2_EndAbility`)))))))))
    (else
      (`self.K2_CancelAbility`)
      (`KismetSystemLibrary.PrintString` "Cannot Commit Sprint"))))

(event `self.K2_OnEndAbility`
  (params (bWasCancelled :type Boolean))
  (`self.K2_HasAuthority`
    (:`True`
      (bind _asbp_character_template (cast `/Game/Blueprints/Core/BP_Character_Template` (`self.GetAvatarActorFromActorInfo`)))
      (bind _state (`/Game/Blueprints/Core/BPI_Character.Get Move State` _asbp_character_template))
      (if (`|EnumEquality` _state "NewEnumerator2")
        (`/Game/Blueprints/Core/BP_Character_Template.Auth Set Move State` _asbp_character_template "NewEnumerator1")
        (`self.BP_RemoveGameplayEffectFromOwnerWithHandle` (`self.EffectHandle`))))))

(fn `K2_CanActivateAbility`
  (params (ActorInfo :type "GameplayAbilityActorInfo Structure") (Handle :type "GameplayAbilitySpecHandle Structure"))
  (returns (RelevantTags :type "GameplayTagContainer Structure") (ReturnValue :type Boolean))
  (bind (_owneractor _avataractor) (break `GameplayAbilityActorInfo` ActorInfo))
  (return (struct) (== (`KismetMathLibrary.MakeRotFromX` (`Actor.GetVelocity` _avataractor)) (`Actor.K2_GetActorRotation` _avataractor) :`ErrorTolerance` 50.0)))