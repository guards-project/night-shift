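; Fire effect actor that spreads Niagara fire over a chosen static mesh from up to three origin points.
; Construction script feeds the mesh, selected fire material and fire, smoke, spark and light settings to three systems, with optional preset origins applied to the first.
; BeginPlay pauses all three.
; FireA/B/C events each unpause one system, set its origin and range, then step its spread time to 1 on a looping timer.
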(event `FireA`
  (params (SpreadSpeed :type "Float (double-precision)") (Location :type "Vector Structure"))
  (bind _dynamic (`self.Dynamic`))
  ;[1 0.005604 0.7584 1 39] To active Fire on first location wire up this Node and Set a World Location and Spread Speed
  (`NiagaraComponent.SetPaused` (`self.Dynamic`) false)
  (bind _returnvalue (`KismetSystemLibrary.K2_SetTimerDelegate` (delegate `timer`) 0.01 true))
  (`NiagaraComponent.SetVariableFloat` _dynamic "Range" (`self.MaxRange`))
  (`NiagaraComponent.SetVariableVec3` _dynamic "locA" Location))

(event `timer`
  ;[1 0.005604 0.7584 1 39] To active Fire on first location wire up this Node and Set a World Location and Spread Speed
  (set `self.time1` (+ (`self.time1`) (/ (stale `FireA` SpreadSpeed) 10.0)))
  (`NiagaraComponent.SetVariableFloat` (`self.Dynamic`) "Time" (`self.time1`))
  (if (>= (`self.time1`) 1.0)
    (`KismetSystemLibrary.K2_ClearAndInvalidateTimerHandle` (stale `FireA` _returnvalue))
    (set `self.time1` 0.0)))

(event `FireB`
  (params (SpreadSpeed :type "Float (double-precision)") (Location :type "Vector Structure"))
  (bind _dynamic2 (`self.Dynamic2`))
  ;[1 0.1248 0.1446 1 39] To active Fire on Second location wire up this Node and Set a World Location and Spread Speed
  (`NiagaraComponent.SetPaused` (`self.Dynamic2`) false)
  (bind _returnvalue (`KismetSystemLibrary.K2_SetTimerDelegate` (delegate `CustomEvent_0`) 0.01 true))
  (`NiagaraComponent.SetVariableFloat` _dynamic2 "Range" (`self.MaxRange`))
  (`NiagaraComponent.SetVariableVec3` _dynamic2 "locB" Location))

(event `CustomEvent_0`
  ;[1 0.1248 0.1446 1 39] To active Fire on Second location wire up this Node and Set a World Location and Spread Speed
  (set `self.time2` (+ (`self.time2`) (/ (stale `FireB` SpreadSpeed) 10.0)))
  (`NiagaraComponent.SetVariableFloat` (`self.Dynamic2`) "Time2" (`self.time2`))
  (if (>= (`self.time2`) 1.0)
    (`KismetSystemLibrary.K2_ClearAndInvalidateTimerHandle` (stale `FireB` _returnvalue))
    (set `self.time2` 0.0)))

(event `self.ReceiveBeginPlay`
  ;[0.1314 1 0.6733 1 20] Paused All Particle System on begin play
  (`NiagaraComponent.SetPaused` (`self.Dynamic`) true)
  (`NiagaraComponent.SetPaused` (`self.Dynamic2`) true)
  (`NiagaraComponent.SetPaused` (`self.Dynamic3`) true))

(event `FireC`
  (params (SpreadSpeed :type "Float (double-precision)") (Location :type "Vector Structure"))
  (bind _dynamic3 (`self.Dynamic3`))
  ;[0 0.2171 1 1 39] To active Fire on third location wire up this Node and Set a World Location and Spread Speed
  (`NiagaraComponent.SetPaused` (`self.Dynamic3`) false)
  (bind _returnvalue (`KismetSystemLibrary.K2_SetTimerDelegate` (delegate `CustomEvent_1`) 0.01 true))
  (`NiagaraComponent.SetVariableFloat` _dynamic3 "Range" (`self.MaxRange`))
  (`NiagaraComponent.SetVariableVec3` _dynamic3 "locC" Location))

(event `CustomEvent_1`
  ;[0 0.2171 1 1 39] To active Fire on third location wire up this Node and Set a World Location and Spread Speed
  (set `self.time3` (+ (`self.time3`) (/ (stale `FireC` SpreadSpeed) 10.0)))
  (`NiagaraComponent.SetVariableFloat` (`self.Dynamic3`) "Time3" (`self.time3`))
  (if (>= (`self.time3`) 1.0)
    (`KismetSystemLibrary.K2_ClearAndInvalidateTimerHandle` (stale `FireC` _returnvalue))
    (set `self.time3` 0.0)))

(fn `UserConstructionScript`
  (bind _dynamic (`self.Dynamic`))
  (bind _dynamic_2 (`self.Dynamic`))
  (bind _dynamic_3 (`self.Dynamic`))
  (bind _dynamic_4 (`self.Dynamic`))
  (bind _dynamic_5 (`self.Dynamic`))
  (bind _dynamic_6 (`self.Dynamic`))
  (bind _dynamic_7 (`self.Dynamic`))
  (`SceneComponent.K2_SetRelativeLocation` (`self.Loca1`) (`self.LocationFire_01`) false false)
  (`SceneComponent.K2_SetRelativeLocation` (`self.Loca2`) (`self.LocationFire_02`) false false)
  (`SceneComponent.K2_SetRelativeLocation` (`self.Loca3`) (`self.LocationFire_03`) false false)
  (`|ExecutionSequence`
    (:`then_0`
      (`StaticMeshComponent.SetStaticMesh` (`self.ImportMesh`) (`self.StaticMesh`))
      (`NiagaraComponent.SetNiagaraVariableObject` (`self.Dynamic`) "StaticMesh" (`self.ImportMesh`))
      (`NiagaraComponent.SetNiagaraVariableObject` (`self.Dynamic2`) "StaticMesh" (`self.ImportMesh`))
      (`NiagaraComponent.SetNiagaraVariableObject` (`self.Dynamic3`) "StaticMesh" (`self.ImportMesh`)))
    (:`then_1`
      (switch `int` (`self.FireType`)
        (:`1`
          (`NiagaraComponent.SetVariableMaterial` _dynamic_2 "FireA" "/Game/FireThrower_Fx/Materials/MI_Fire_Inst_Smoke_AA.MI_Fire_Inst_Smoke_AA")
          (`NiagaraComponent.SetVariableMaterial` (`self.Dynamic2`) "FireA" "/Game/FireThrower_Fx/Materials/MI_Fire_Inst_Smoke_AA.MI_Fire_Inst_Smoke_AA")
          (`NiagaraComponent.SetVariableMaterial` (`self.Dynamic3`) "FireA" "/Game/FireThrower_Fx/Materials/MI_Fire_Inst_Smoke_AA.MI_Fire_Inst_Smoke_AA")
          (`NiagaraComponent.SetVariableMaterial` _dynamic_2 "FireB" "/Game/FireThrower_Fx/Materials/M_None.M_None")
          (`NiagaraComponent.SetVariableMaterial` (`self.Dynamic2`) "FireB" "/Game/FireThrower_Fx/Materials/M_None.M_None")
          (`NiagaraComponent.SetVariableMaterial` (`self.Dynamic3`) "FireB" "/Game/FireThrower_Fx/Materials/M_None.M_None")
          (`NiagaraComponent.SetVariableMaterial` _dynamic_2 "FireC" "/Game/FireThrower_Fx/Materials/M_None.M_None")
          (`NiagaraComponent.SetVariableMaterial` (`self.Dynamic2`) "FireC" "/Game/FireThrower_Fx/Materials/M_None.M_None")
          (`NiagaraComponent.SetVariableMaterial` (`self.Dynamic3`) "FireC" "/Game/FireThrower_Fx/Materials/M_None.M_None")
          (`NiagaraComponent.SetVariableMaterial` _dynamic_2 "FireD" "/Game/FireThrower_Fx/Materials/M_None.M_None")
          (`NiagaraComponent.SetVariableMaterial` (`self.Dynamic2`) "FireD" "/Game/FireThrower_Fx/Materials/M_None.M_None")
          (`NiagaraComponent.SetVariableMaterial` (`self.Dynamic3`) "FireD" "/Game/FireThrower_Fx/Materials/M_None.M_None"))
        (:`2`
          (`NiagaraComponent.SetVariableMaterial` _dynamic_2 "FireA" "/Game/FireThrower_Fx/Materials/M_None.M_None")
          (`NiagaraComponent.SetVariableMaterial` (`self.Dynamic2`) "FireA" "/Game/FireThrower_Fx/Materials/M_None.M_None")
          (`NiagaraComponent.SetVariableMaterial` (`self.Dynamic3`) "FireA" "/Game/FireThrower_Fx/Materials/M_None.M_None")
          (`NiagaraComponent.SetVariableMaterial` _dynamic_2 "FireB" "/Game/FireThrower_Fx/Materials/MI_Fire_Inst_Smoke_BB.MI_Fire_Inst_Smoke_BB")
          (`NiagaraComponent.SetVariableMaterial` (`self.Dynamic2`) "FireB" "/Game/FireThrower_Fx/Materials/MI_Fire_Inst_Smoke_BB.MI_Fire_Inst_Smoke_BB")
          (`NiagaraComponent.SetVariableMaterial` (`self.Dynamic3`) "FireB" "/Game/FireThrower_Fx/Materials/MI_Fire_Inst_Smoke_BB.MI_Fire_Inst_Smoke_BB")
          (`NiagaraComponent.SetVariableMaterial` _dynamic_2 "FireC" "/Game/FireThrower_Fx/Materials/M_None.M_None")
          (`NiagaraComponent.SetVariableMaterial` (`self.Dynamic2`) "FireC" "/Game/FireThrower_Fx/Materials/M_None.M_None")
          (`NiagaraComponent.SetVariableMaterial` (`self.Dynamic3`) "FireC" "/Game/FireThrower_Fx/Materials/M_None.M_None")
          (`NiagaraComponent.SetVariableMaterial` _dynamic_2 "FireD" "/Game/FireThrower_Fx/Materials/M_None.M_None")
          (`NiagaraComponent.SetVariableMaterial` (`self.Dynamic2`) "FireD" "/Game/FireThrower_Fx/Materials/M_None.M_None")
          (`NiagaraComponent.SetVariableMaterial` (`self.Dynamic3`) "FireD" "/Game/FireThrower_Fx/Materials/M_None.M_None"))
        (:`3`
          (`NiagaraComponent.SetVariableMaterial` _dynamic_2 "FireA" "/Game/FireThrower_Fx/Materials/M_None.M_None")
          (`NiagaraComponent.SetVariableMaterial` (`self.Dynamic2`) "FireA" "/Game/FireThrower_Fx/Materials/M_None.M_None")
          (`NiagaraComponent.SetVariableMaterial` (`self.Dynamic3`) "FireA" "/Game/FireThrower_Fx/Materials/M_None.M_None")
          (`NiagaraComponent.SetVariableMaterial` _dynamic_2 "FireB" "/Game/FireThrower_Fx/Materials/M_None.M_None")
          (`NiagaraComponent.SetVariableMaterial` (`self.Dynamic2`) "FireB" "/Game/FireThrower_Fx/Materials/M_None.M_None")
          (`NiagaraComponent.SetVariableMaterial` (`self.Dynamic3`) "FireB" "/Game/FireThrower_Fx/Materials/M_None.M_None")
          (`NiagaraComponent.SetVariableMaterial` _dynamic_2 "FireC" "/Game/FireThrower_Fx/Materials/MI_Fire_Inst_Smoke_CC.MI_Fire_Inst_Smoke_CC")
          (`NiagaraComponent.SetVariableMaterial` (`self.Dynamic2`) "FireC" "/Game/FireThrower_Fx/Materials/MI_Fire_Inst_Smoke_CC.MI_Fire_Inst_Smoke_CC")
          (`NiagaraComponent.SetVariableMaterial` (`self.Dynamic3`) "FireC" "/Game/FireThrower_Fx/Materials/MI_Fire_Inst_Smoke_CC.MI_Fire_Inst_Smoke_CC")
          (`NiagaraComponent.SetVariableMaterial` _dynamic_2 "FireD" "/Game/FireThrower_Fx/Materials/M_None.M_None")
          (`NiagaraComponent.SetVariableMaterial` (`self.Dynamic2`) "FireD" "/Game/FireThrower_Fx/Materials/M_None.M_None")
          (`NiagaraComponent.SetVariableMaterial` (`self.Dynamic3`) "FireD" "/Game/FireThrower_Fx/Materials/M_None.M_None"))
        (:`4`
          (`NiagaraComponent.SetVariableMaterial` _dynamic_2 "FireA" "/Game/FireThrower_Fx/Materials/M_None.M_None")
          (`NiagaraComponent.SetVariableMaterial` (`self.Dynamic2`) "FireA" "/Game/FireThrower_Fx/Materials/M_None.M_None")
          (`NiagaraComponent.SetVariableMaterial` (`self.Dynamic3`) "FireA" "/Game/FireThrower_Fx/Materials/M_None.M_None")
          (`NiagaraComponent.SetVariableMaterial` _dynamic_2 "FireB" "/Game/FireThrower_Fx/Materials/M_None.M_None")
          (`NiagaraComponent.SetVariableMaterial` (`self.Dynamic2`) "FireB" "/Game/FireThrower_Fx/Materials/M_None.M_None")
          (`NiagaraComponent.SetVariableMaterial` (`self.Dynamic3`) "FireB" "/Game/FireThrower_Fx/Materials/M_None.M_None")
          (`NiagaraComponent.SetVariableMaterial` _dynamic_2 "FireC" "/Game/FireThrower_Fx/Materials/M_None.M_None")
          (`NiagaraComponent.SetVariableMaterial` (`self.Dynamic2`) "FireC" "/Game/FireThrower_Fx/Materials/M_None.M_None")
          (`NiagaraComponent.SetVariableMaterial` (`self.Dynamic3`) "FireC" "/Game/FireThrower_Fx/Materials/M_None.M_None")
          (`NiagaraComponent.SetVariableMaterial` _dynamic_2 "FireD" "/Game/FireThrower_Fx/Materials/MI_Fire_Inst_Smoke_DD.MI_Fire_Inst_Smoke_DD")
          (`NiagaraComponent.SetVariableMaterial` (`self.Dynamic2`) "FireD" "/Game/FireThrower_Fx/Materials/MI_Fire_Inst_Smoke_DD.MI_Fire_Inst_Smoke_DD")
          (`NiagaraComponent.SetVariableMaterial` (`self.Dynamic3`) "FireD" "/Game/FireThrower_Fx/Materials/MI_Fire_Inst_Smoke_DD.MI_Fire_Inst_Smoke_DD"))))
    (:`then_2`
      (`NiagaraComponent.SetVariableFloat` _dynamic_6 "Contrast" (`self.Contrast`))
      (`NiagaraComponent.SetVariableFloat` (`self.Dynamic2`) "Contrast" (`self.Contrast`))
      (`NiagaraComponent.SetVariableFloat` (`self.Dynamic3`) "Contrast" (`self.Contrast`))
      (`NiagaraComponent.SetVariableFloat` _dynamic_6 "Emessive" (`self.Emessive`))
      (`NiagaraComponent.SetVariableFloat` (`self.Dynamic2`) "Emessive" (`self.Emessive`))
      (`NiagaraComponent.SetVariableFloat` (`self.Dynamic3`) "Emessive" (`self.Emessive`))
      (`NiagaraComponent.SetVariableFloat` _dynamic_6 "Opacity" (`self.Opacity`))
      (`NiagaraComponent.SetVariableFloat` (`self.Dynamic2`) "Opacity" (`self.Opacity`))
      (`NiagaraComponent.SetVariableFloat` (`self.Dynamic3`) "Opacity" (`self.Opacity`))
      (`NiagaraComponent.SetVariableFloat` _dynamic_6 "Temperature" (`self.temperature`))
      (`NiagaraComponent.SetVariableFloat` (`self.Dynamic2`) "Temperature" (`self.temperature`))
      (`NiagaraComponent.SetVariableFloat` (`self.Dynamic3`) "Temperature" (`self.temperature`))
      (`NiagaraComponent.SetVariableFloat` _dynamic_6 "Lifetime" (`self.Lifetime`))
      (`NiagaraComponent.SetVariableFloat` (`self.Dynamic2`) "Lifetime" (`self.Lifetime`))
      (`NiagaraComponent.SetVariableFloat` (`self.Dynamic3`) "Lifetime" (`self.Lifetime`))
      (`NiagaraComponent.SetVariableFloat` _dynamic_6 "Scale_max" (`self.Scale_max`))
      (`NiagaraComponent.SetVariableFloat` (`self.Dynamic2`) "Scale_max" (`self.Scale_max`))
      (`NiagaraComponent.SetVariableFloat` (`self.Dynamic3`) "Scale_max" (`self.Scale_max`))
      (`NiagaraComponent.SetVariableFloat` _dynamic_6 "SpawnRate" (`self.SpawnRate`))
      (`NiagaraComponent.SetVariableFloat` (`self.Dynamic2`) "SpawnRate" (`self.SpawnRate`))
      (`NiagaraComponent.SetVariableFloat` (`self.Dynamic3`) "SpawnRate" (`self.SpawnRate`))
      (`NiagaraComponent.SetVariableFloat` _dynamic_6 "FireTimeBurn" (`self.FireTimeBurn`))
      (`NiagaraComponent.SetVariableFloat` (`self.Dynamic2`) "FireTimeBurn" (`self.FireTimeBurn`))
      (`NiagaraComponent.SetVariableFloat` (`self.Dynamic3`) "FireTimeBurn" (`self.FireTimeBurn`))
      (`NiagaraComponent.SetVariableFloat` _dynamic_7 "SparkRate" (`self.SparkRate`))
      (`NiagaraComponent.SetVariableFloat` (`self.Dynamic2`) "SparkRate" (`self.SparkRate`))
      (`NiagaraComponent.SetVariableFloat` (`self.Dynamic3`) "SparkRate" (`self.SparkRate`))
      (`NiagaraComponent.SetVariableFloat` _dynamic_7 "SparkSize" (`self.SparkSize`))
      (`NiagaraComponent.SetVariableFloat` (`self.Dynamic2`) "SparkSize" (`self.SparkSize`))
      (`NiagaraComponent.SetVariableFloat` (`self.Dynamic3`) "SparkSize" (`self.SparkSize`))
      (`NiagaraComponent.SetVariableLinearColor` _dynamic_7 "Smoke_Color" (`self.Smoke_Color`))
      (`NiagaraComponent.SetVariableLinearColor` (`self.Dynamic3`) "Smoke_Color" (`self.Smoke_Color`))
      (`NiagaraComponent.SetVariableFloat` _dynamic_7 "SpawnSmokeRate" (`self.SpawnSmokeRate`))
      (`NiagaraComponent.SetVariableFloat` (`self.Dynamic2`) "SpawnSmokeRate" (`self.SpawnSmokeRate`))
      (`NiagaraComponent.SetVariableFloat` (`self.Dynamic3`) "SpawnSmokeRate" (`self.SpawnSmokeRate`))
      (`NiagaraComponent.SetVariableFloat` _dynamic_7 "LifeTimeSmoke" (`self.LifeTimeSmoke`))
      (`NiagaraComponent.SetVariableFloat` (`self.Dynamic2`) "LifeTimeSmoke" (`self.LifeTimeSmoke`))
      (`NiagaraComponent.SetVariableFloat` (`self.Dynamic3`) "LifeTimeSmoke" (`self.LifeTimeSmoke`))
      (`NiagaraComponent.SetVariableFloat` _dynamic_7 "SmokeSize" (`self.SmokeSize`))
      (`NiagaraComponent.SetVariableFloat` (`self.Dynamic2`) "SmokeSize" (`self.SmokeSize`))
      (`NiagaraComponent.SetVariableFloat` (`self.Dynamic3`) "SmokeSize" (`self.SmokeSize`))
      (`NiagaraComponent.SetVariableLinearColor` _dynamic_7 "Light_Color" (`self.light_Color`))
      (`NiagaraComponent.SetVariableLinearColor` (`self.Dynamic2`) "Light_Color" (`self.light_Color`))
      (`NiagaraComponent.SetVariableLinearColor` (`self.Dynamic3`) "Light_Color" (`self.light_Color`))
      (`NiagaraComponent.SetVariableFloat` _dynamic_5 "Light_intensity" (`self.Light_intensity`))
      (`NiagaraComponent.SetVariableFloat` (`self.Dynamic2`) "Light_intensity" (`self.Light_intensity`))
      (`NiagaraComponent.SetVariableFloat` (`self.Dynamic3`) "Light_intensity" (`self.Light_intensity`))
      (`NiagaraComponent.SetVariableFloat` _dynamic_5 "Light_Radius" (`self.Light_Radius`))
      (`NiagaraComponent.SetVariableFloat` (`self.Dynamic2`) "Light_Radius" (`self.Light_Radius`))
      (`NiagaraComponent.SetVariableFloat` (`self.Dynamic3`) "Light_Radius" (`self.Light_Radius`))
      (`NiagaraComponent.SetVariableFloat` _dynamic_5 "Light_SpawnRate" (`self.Light_SpawnRate`))
      (`NiagaraComponent.SetVariableFloat` (`self.Dynamic2`) "Light_SpawnRate" (`self.Light_SpawnRate`))
      (`NiagaraComponent.SetVariableFloat` (`self.Dynamic3`) "Light_SpawnRate" (`self.Light_SpawnRate`))
      (`NiagaraComponent.SetVariableFloat` _dynamic_5 "Scale_min" (`self.Scale_min`))
      (`NiagaraComponent.SetVariableFloat` (`self.Dynamic2`) "Scale_min" (`self.Scale_min`))
      (`NiagaraComponent.SetVariableFloat` (`self.Dynamic3`) "Scale_min" (`self.Scale_min`)))
    (:`then_3`
      (`|ExecutionSequence`
        (:`then_0`
          (if (`self.Location_01`)
            (`NiagaraComponent.SetVariableFloat` _dynamic_3 "Range" (`self.MaxRange`))
            (`NiagaraComponent.SetVariableVec3` _dynamic_3 "locA" (`SceneComponent.K2_GetComponentLocation` (`self.Loca1`)))
            (`NiagaraComponent.SetVariableFloat` _dynamic_3 "Time" (`self.Time_01`))))
        (:`then_1`
          (if (`self.Location_02`)
            (`NiagaraComponent.SetVariableFloat` _dynamic_4 "Range" (`self.MaxRange`))
            (`NiagaraComponent.SetVariableFloat` _dynamic_4 "Time2" (`self.Time_02`))
            (`NiagaraComponent.SetVariableVec3` _dynamic_4 "locB" (`SceneComponent.K2_GetComponentLocation` (`self.Loca2`)))))
        (:`then_2`
          (if (`self.Location_03`)
            (`NiagaraComponent.SetVariableFloat` _dynamic "Range" (`self.MaxRange`))
            (`NiagaraComponent.SetVariableVec3` _dynamic "locC" (`SceneComponent.K2_GetComponentLocation` (`self.Loca3`)))
            (`NiagaraComponent.SetVariableFloat` _dynamic "Time3" (`self.Time_03`))))))))