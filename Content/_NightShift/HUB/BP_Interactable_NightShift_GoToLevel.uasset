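; Hub interactable for Night Shift that starts a mission by sending the game to a configured level.
; Only the server or a standalone game can interact with it, under the prompt "Start Mission".
; On interaction, the authority casts the game state to BP_GameState_Guards and passes LevelName to its GoToLevel function.
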(event `/Game/Primer/Primer_Interaction/BPI_Interact.Execute Interact`
  (params (User :type "Controller Object Reference"))
  (`/Engine/EditorBlueprintResources/ActorMacros.Switch Has Authority`
    (:`Authority`
      (bind _asbp_game_state_guards (cast `/Game/Blueprints/Core/BP_GameState_Guards` (`GameplayStatics.GetGameState`)))
      (`/Game/Blueprints/Core/BP_GameState_Guards.Go to Level` _asbp_game_state_guards (`self.Level Name`)))))

(fn `Get Can Interact`
  (returns (ReturnValue :type Boolean))
  (return (or (`KismetSystemLibrary.IsServer`) (`KismetSystemLibrary.IsStandalone`))))

(fn `Get Interact Text`
  (returns (Text :type Text))
  (return "Start Mission"))

(fn `UserConstructionScript`
  (`parent.UserConstructionScript`))