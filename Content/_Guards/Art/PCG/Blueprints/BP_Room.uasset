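; BP_Room is a spline-outlined room Blueprint, filed with the PCG art assets.
; Its construction script zeroes local tangents and sets every spline point to linear, keeping the outline straight-edged with sharp corners.
; It then derives a RoofScale vector from ShowCeiling, giving either a Z-stretched scale or zero when the ceiling is hidden.
; The event graph holds no active logic.
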(event EventBeginPlay)

(event Collision|EventActorBeginOverlap
  (params (OtherActor :type Actor%20Object%20Reference)))

(event EventTick
  (params (DeltaSeconds :type Float%20%28single-precision%29)))

(fn ConstructionScript
  (CallFunction|FixSpline)
  (Variables|Default|SetRoof%20Scale (Math|Vector|SelectVector "1.000000,1.000000,15.000000" "0, 0, 0" (Variables|Default|GetShow%20Ceiling))))

(fn FixSpline
  (bind _returnvalue (Math|Vector|MakeVector 0.0 0.0 0.0))
  (bind _spline (Variables|Default|GetSpline))
  (for _index (range 0 (- (Spline|GetNumberOfSplinePoints (Variables|Default|GetSpline)) 1))
    (Spline|SetTangentsatSplinePoint _spline _index _returnvalue _returnvalue "Local" true)
    (Spline|SetSplinePointType _spline _index "Linear" true))
  (Spline|UpdateSpline _spline))