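; Custom PCG element that generates a centred grid of points, each rotated to look at the grid centre.
; Grid extents and cell size set the count for a 3D volume or an XY, XZ or YZ plane.
; An IterationLoop derives each position from its index and seeds the point from it.
; In local mode, it composes with the owning actor's transform, optionally culls by spatial-data density, and can output untransformed positions.
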(fn ExecutewithContext
  (params (InContext :type PCG%20Context%20Structure%20%28by%20ref%29) (Input :type PCG%20Data%20Collection%20Structure%20%28by%20ref%29))
  (bind _gridextents (Variables|Default|GetGridExtents))
  (bind _cell_size (Variables|Default|GetCell%20Size))
  (bind _returnvalue (* _gridextents 2.0))
  (bind _returnvalue_2 (/ _returnvalue _cell_size))
  (bind _returnvalue_3 (Class|KismetMathLibrary|FTruncVector _returnvalue_2))
  (bind (_x _y _z) (Utilities|Struct|BreakIntVector _returnvalue_3))
  (bind _output_get (LocalVariables|SetContext InContext))
  (bind _returnvalue_4 (PCG|Temporary|GetActorData _output_get))
  (bind _aspcgspatial_data (Utilities|Casting|CastToPCGSpatialData _returnvalue_4))
  (Variables|Private|SetContext%20PCGSpatial%20Data _aspcgspatial_data)
  (LocalVariables|SetTarget%20Actor (Variables|/Script/PCG.PCGSpatialData|GetTargetActor _aspcgspatial_data))
  (Utilities|Array|Clear (LocalVariables|GetOutPoints))
  (Variables|Private|SetIncrementSize (Math|Vector|VectorGetAbs _cell_size))
  (Variables|Private|SetIncrements _returnvalue_3)
  (bind _outdata (PCG|FlowControl|IterationLoop (LocalVariables|GetContext) (Class|KismetMathLibrary|ToInt64(Integer) (Math|Integer|SelectInt (* _x _y _z) (Utilities|Select :Index (Variables|Default|GetCoordinate%20Plane%20Axes) :NewEnumerator0 (* _x _y) :NewEnumerator2 (* _x _z) :NewEnumerator3 (* _y _z)) (Variables|Default|GetVolume))) 0 0 0))
  (Variables|/Script/PCG.PCGSpatialData|SetTargetActor _outdata (LocalVariables|GetTarget%20Actor))
  (return (Utilities|Struct|MakePCGDataCollection (Utilities|Array|MakeArray (Utilities|Struct|MakePCGTaggedData _outdata 0 "None")))))

(fn IterationLoopBody
  (params (InContext :type PCG%20Context%20Structure%20%28by%20ref%29) (Iteration :type Integer64) (InA :type PCG%20Spatial%20Data%20Object%20Reference) (InB :type PCG%20Spatial%20Data%20Object%20Reference) (OutMetadata :type PCG%20Metadata%20Object%20Reference))
  (bind _returnvalue (Math|Conversions|ToInteger(Byte) Iteration))
  (bind _gridcenterposition (Variables|Default|GetGridCenterPosition))
  (bind _cell_size (Variables|Default|GetCell%20Size))
  (bind _coordinate_plane_axes (Variables|Default|GetCoordinate%20Plane%20Axes))
  (bind _coordinate_plane_axes_2 (Variables|Default|GetCoordinate%20Plane%20Axes))
  (bind _volume (Variables|Default|GetVolume))
  (bind _coordinate_plane_axes_3 (Variables|Default|GetCoordinate%20Plane%20Axes))
  (bind _volume_2 (Variables|Default|GetVolume))
  (bind _gridcenterposition_2 (Variables|Default|GetGridCenterPosition))
  (bind _volume_3 (Variables|Default|GetVolume))
  (bind _increments (Variables|Private|GetIncrements))
  (bind _increments_2 (Variables|Private|GetIncrements))
  (bind _increments_3 (Variables|Private|GetIncrements))
  (bind _incrementsize (Variables|Private|GetIncrementSize))
  (bind (_x _y _z) (Utilities|Struct|BreakIntVector _increments_3))
  (bind (_x_2 _y_2 _z_2) (Utilities|Struct|BreakIntVector _increments_3))
  (bind _returnvalue_2 (* _incrementsize "0.000000,0.000000,1.000000"))
  (bind _returnvalue_3 (* _cell_size _increments))
  (bind _returnvalue_4 (Utilities|Select :Index _coordinate_plane_axes_3 :NewEnumerator0 "0,1.000000, 0" :NewEnumerator2 "0, 0,1.000000" :NewEnumerator3 "0, 0,1.000000"))
  (bind _returnvalue_5 (Utilities|Select :Index _coordinate_plane_axes_3 :NewEnumerator0 "1.000000, 0, 0" :NewEnumerator2 "1.000000,0.000000, 0" :NewEnumerator3 "0,1.000000, 0"))
  (bind _returnvalue_6 (Utilities|Select :Index _coordinate_plane_axes_2 :NewEnumerator0 "1.000000,1.000000, 0" :NewEnumerator2 "1.000000,0.000000,1.000000" :NewEnumerator3 "0.000000,1.000000,1.000000"))
  (bind _returnvalue_7 (Math|Vector|SelectVector "0,1.000000, 0" _returnvalue_4 _volume_2))
  (bind _returnvalue_8 (Math|Vector|SelectVector "1.000000, 0, 0" _returnvalue_5 _volume_2))
  (bind _intvector (Utilities|Struct|MakeIntVector _y _z))
  (bind _intvector_2 (Utilities|Struct|MakeIntVector _x_2 _z_2))
  (bind _returnvalue_9 (- _returnvalue_3 _cell_size))
  (bind _returnvalue_10 (/ _returnvalue_9 2.0))
  (bind _returnvalue_11 (* _incrementsize _returnvalue_8))
  (bind _returnvalue_12 (* _incrementsize _returnvalue_7))
  (bind _returnvalue_13 (Utilities|Select :Index _coordinate_plane_axes :NewEnumerator0 _increments_3 :NewEnumerator2 _intvector_2 :NewEnumerator3 _intvector))
  (bind _returnvalue_14 (select _volume_3 _increments_2 _returnvalue_13))
  (bind (_x_3 _y_3) (Utilities|Struct|BreakIntVector _returnvalue_14))
  (bind _returnvalue_15 (Math|Integer|%(Integer) _returnvalue _x_3))
  (bind _returnvalue_16 (/ _returnvalue _x_3))
  (bind _returnvalue_17 (* _x_3 _y_3))
  (bind _returnvalue_18 (Math|Integer|%(Integer) _returnvalue_16 _y_3))
  (bind _returnvalue_19 (/ _returnvalue _returnvalue_17))
  (bind _returnvalue_20 (* _returnvalue_11 _returnvalue_15))
  (bind _returnvalue_21 (* _returnvalue_12 _returnvalue_18))
  (bind _returnvalue_22 (* _returnvalue_2 _returnvalue_19))
  (bind _returnvalue_23 (+ _returnvalue_20 _returnvalue_21))
  (bind _returnvalue_24 (+ _returnvalue_23 _returnvalue_22))
  (bind _returnvalue_25 (- _returnvalue_24 _returnvalue_10))
  (bind _returnvalue_26 (* _returnvalue_25 _returnvalue_6))
  (bind _returnvalue_27 (Math|Vector|SelectVector _returnvalue_25 _returnvalue_26 _volume))
  (bind _returnvalue_28 (+ _returnvalue_27 _gridcenterposition_2))
  (bind _returnvalue_29 (Math|Rotator|FindLookatRotation _returnvalue_28 _gridcenterposition))
  (bind _returnvalue_30 (Math|Transform|MakeTransform _returnvalue_28 _returnvalue_29))
  (bind (_location _rotation _scale) (Math|Transform|BreakTransform _returnvalue_30))
  (if (Variables|Default|GetLocal)
    (bind _returnvalue_31 (PCG|Temporary|GetOriginalComponent InContext))
    (if (select (Variables|Default|GetCullPointsOutsideVolume) (> (Distribution|GetDensityatPosition (Variables|Private|GetContext%20PCGSpatial%20Data) (.Location (Math|Transform|BreakTransform (Math|Transform|ComposeTransforms _returnvalue_30 (Math|Transform|MakeTransform (.Location (Math|Transform|BreakTransform (Transformation|GetActorTransform (Components|GetOwner _returnvalue_31)))) (.Rotation (Math|Transform|BreakTransform (Transformation|GetActorTransform (Components|GetOwner _returnvalue_31))))))))) 0.0) true)
      (if (Variables|Default|GetLocal%20Inverse%20Transform)
        (bind _returnvalue_32 (PCG|Helpers|ComputeSeedfromPosition (.Location (Math|Transform|BreakTransform _returnvalue_30))))
        (return (Utilities|Struct|MakePCGPoint (Math|Transform|MakeTransform _location (Math|Rotator|FindLookatRotation _location (Variables|Default|GetGridCenterPosition)) _scale) "-1.000000,-1.000000,-1.000000" "1.000000,1.000000,1.000000" _returnvalue_32) true)
        (else
          (bind _returnvalue_33 (PCG|Helpers|ComputeSeedfromPosition (.Location (Math|Transform|BreakTransform (Math|Transform|ComposeTransforms _returnvalue_30 (Math|Transform|MakeTransform (.Location (Math|Transform|BreakTransform (Transformation|GetActorTransform (Components|GetOwner _returnvalue_31)))) (.Rotation (Math|Transform|BreakTransform (Transformation|GetActorTransform (Components|GetOwner _returnvalue_31))))))))))
          (return (Utilities|Struct|MakePCGPoint (Math|Transform|MakeTransform (.Location (Math|Transform|BreakTransform (Math|Transform|ComposeTransforms _returnvalue_30 (Math|Transform|MakeTransform (.Location (Math|Transform|BreakTransform (Transformation|GetActorTransform (Components|GetOwner _returnvalue_31)))) (.Rotation (Math|Transform|BreakTransform (Transformation|GetActorTransform (Components|GetOwner _returnvalue_31)))))))) (Math|Rotator|FindLookatRotation (.Location (Math|Transform|BreakTransform (Math|Transform|ComposeTransforms _returnvalue_30 (Math|Transform|MakeTransform (.Location (Math|Transform|BreakTransform (Transformation|GetActorTransform (Components|GetOwner _returnvalue_31)))) (.Rotation (Math|Transform|BreakTransform (Transformation|GetActorTransform (Components|GetOwner _returnvalue_31)))))))) (Variables|Default|GetGridCenterPosition)) (.Scale (Math|Transform|BreakTransform (Math|Transform|ComposeTransforms _returnvalue_30 (Math|Transform|MakeTransform (.Location (Math|Transform|BreakTransform (Transformation|GetActorTransform (Components|GetOwner _returnvalue_31)))) (.Rotation (Math|Transform|BreakTransform (Transformation|GetActorTransform (Components|GetOwner _returnvalue_31))))))))) "-1.000000,-1.000000,-1.000000" "1.000000,1.000000,1.000000" _returnvalue_33) true))))
    (else
      (bind _returnvalue_34 (PCG|Helpers|ComputeSeedfromPosition _returnvalue_28))
      (return (Utilities|Struct|MakePCGPoint _returnvalue_30 "-1.000000,-1.000000,-1.000000" "1.000000,1.000000,1.000000" _returnvalue_34) (select (Variables|Default|GetCullPointsOutsideVolume) (> (Distribution|GetDensityatPosition (Variables|Private|GetContext%20PCGSpatial%20Data) _returnvalue_28) 0.0) true)))))

(fn NodeTitleOverride
  (return "Create Points Grid Look At"))