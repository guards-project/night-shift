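; Custom PCG node that assigns each point a random mesh from a named mesh set on the PCG owner's BP_PCGMeshSet_Component.
; It expands the set into a weighted bag by repeating each mesh by its count.
; A point loop writes a seed-stable pick to the "Mesh" string attribute, returning after the first "In" data.
; Without a component or meshes, the input passes through unchanged.
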(fn ExecutewithContext
  (params (InContext :type PCG%20Context%20Structure%20%28by%20ref%29) (Input :type PCG%20Data%20Collection%20Structure%20%28by%20ref%29))
  (Utilities|FlowControl|Sequence
    (:then_0
      ;[1 1 1] Get mesh data from BP component
      (bind _returnvalue (PCG|Temporary|GetComponent InContext))
      (Utilities|IsValid (Actor|GetComponentbyClass (Components|GetOwner _returnvalue) "/Game/_Guards/Art/PCG/Blueprints/BP_PCGMeshSet_Component.BP_PCGMeshSet_Component_C")
        (:Is%20Valid
          (bind _meshes (Default|GetMeshSetbyName (Actor|GetComponentbyClass (Components|GetOwner _returnvalue) "/Game/_Guards/Art/PCG/Blueprints/BP_PCGMeshSet_Component.BP_PCGMeshSet_Component_C") (Variables|Default|GetSet%20Name)))
          (PCG|Execution|CreateMeshBag _meshes)
          (if (> (Utilities|Map|Length _meshes) 0)
            ;[1 1 1] Add Mesh Attribute to points and perform a point loop
            (bind _returnvalue_2 (Class|PCGDataFunctionLibrary|GetInputsbyPin Input (Utilities|Name|MakeLiteralName "In")))
            (for _array_element _returnvalue_2
              (bind _aspcgspatial_data (Utilities|Casting|CastToPCGSpatialData (.Data (Utilities|Struct|BreakPCGTaggedData _array_element))))
              (bind _returnvalue_3 (Metadata|MutableMetadata _aspcgspatial_data))
              (PCG|Metadata|CreateStringAttribute _returnvalue_3 "Mesh" (Variables|Default|GetDefault%20Mesh%20Path) false true)
              (bind _outdata (PCG|FlowControl|PointLoop InContext (SpatialData|ToPointDatawithContext _aspcgspatial_data InContext) 0))
              (return (Utilities|Struct|MakePCGDataCollection (Utilities|Array|MakeArray (Utilities|Struct|MakePCGTaggedData _outdata 0 "None")))))))))
    (:then_1
      (return Input))))

(fn PointLoopBody
  (params (InContext :type PCG%20Context%20Structure%20%28by%20ref%29) (InData :type PCG%20Point%20Data%20Object%20Reference) (InPoint :type PCG%20Point%20Structure%20%28by%20ref%29) (OutMetadata :type PCG%20Metadata%20Object%20Reference))
  (bind _mesh_bag (Variables|Default|GetMesh%20Bag))
  (Class|PCGMetadataAccessorHelpers|SetStringAttribute InPoint OutMetadata "Mesh" (Utilities|ToString(SoftObjectReference) (Utilities|Array|Get(acopy) _mesh_bag (Math|Random|RandomIntegerinRangefromStream (Math|Random|MakeRandomStream (Utilities|Struct|BreakPCGPoint InPoint)) 0 (Utilities|Array|LastIndex _mesh_bag)))))
  (return InPoint true))

(fn CreateMeshBag
  (params (TargetMap :type Map%20of%20Static%20Mesh%20Soft%20Object%20References%20to%20Integers))
  (bind _keys (Utilities|Map|Keys TargetMap))
  (for _array_element _keys
    (for _index (range 0 (- (.Value (Utilities|Map|Find TargetMap _array_element)) 1))
      (Utilities|Array|Add (Variables|Default|GetMesh%20Bag) _array_element))))