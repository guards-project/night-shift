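; BP_DangerCircle is a decal telegraph that shows a danger area filling up, then plays an explosion effect when time runs out.
; On BeginPlay, the Grow timeline, rate-scaled by Duration, enlarges DecalGrow alongside DecalBase.
; When finished, it spawns the Niagara explosion and boss attack sound, hides both decals, and destroys itself after a short delay on authority only.
; It applies no damage itself.
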(event `self.ReceiveBeginPlay`
  (`TimelineComponent.SetPlayRate` (`self.Grow`) (/ 1.0 (`self.Duration`)))
  (bind (_direction _alpha) (`Timeline|Grow` :!via `PlayFromStart`)
    (:`Update`
      (`SceneComponent.SetWorldScale3D` (`self.DecalGrow`) (`KismetMathLibrary.VLerp` (0.1 0.1 0.1) (0.1 1.5 1.5) _alpha)))
    (:`Finished`
      (`NiagaraFunctionLibrary.SpawnSystemAtLocation` "/Game/_Guards/Art/Materials/Decals/NS_DangerExplosion.NS_DangerExplosion" (`self.K2_GetActorLocation`))
      (`GameplayStatics.PlaySoundAtLocation` "/Game/_Guards/Audio/Sounds/A_D3BossAttack.A_D3BossAttack" (`self.K2_GetActorLocation`) (struct) 1.0 1.0 0.0 null null null null)
      (`SceneComponent.SetVisibility` (`self.DecalGrow`) false false)
      (`SceneComponent.SetVisibility` (`self.DecalBase`) false false)
      (`/Engine/EditorBlueprintResources/ActorMacros.Switch Has Authority`
        (:`Authority`
          (`KismetSystemLibrary.Delay` 2.0)
          (`self.K2_DestroyActor`))))))

(fn `UserConstructionScript`)