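; BP_AchievementProgressor is a short-lived actor that increments an online subsystem user stat and advances its linked achievement.
; On BeginPlay it requests current stats, then in a one-shot callback applies the increment and stores stats only for listed names.
; It then writes the achievement through the player controller's achievement component at max progress, or shows progress at selected milestones.
; It destroys itself after either outcome.
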(event `self.ReceiveBeginPlay`
  ;[0.2026 0.5578 1] Update Stats to get latest, then unbind from that event and increment. Draw achievement if complete.
  (if (`/Game/_Guards/OnlineSubsystem/BPFL_OnlineSubsystem.Guards Has Online Subsystem`)
    (`/Game/_Guards/OnlineSubsystem/BPFL_OnlineSubsystem.Request Stats` (delegate `Stat Callback`))
    (else
      (`self.K2_DestroyActor`))))

(event `Stat Callback`
  (params (Data :type "UserStatsReceived Structure (by ref)"))
  ;[0.2026 0.5578 1] Update Stats to get latest, then unbind from that event and increment. Draw achievement if complete.
  (`/Engine/EditorBlueprintResources/StandardMacros.DoOnce` false
    (:`Completed`
      (remove `UserStats.UserStatsReceived` (subsystem `UserStats`) (delegate `Stat Callback`))
      (bind _data (`UserStats.GetStatInt` (`self.Stat Name`)))
      (set `self.Stat` _data)
      (if (> (`self.Increment Amount`) 0)
        (`UserStats.SetStatInt` (`self.Stat Name`) (+ (`self.Stat`) (`self.Increment Amount`)))
        (bind _data_2 (`UserStats.GetStatInt` (`self.Stat Name`)))
        (set `self.Stat` _data_2)
        (`self.Try Store Stats`)
        (`self.Process Achievement`)
        (else
          (`self.Process Achievement`))))))

(event `Process Achievement`
  (bind _stat (`self.Stat`))
  ;[0.2026 0.5578 1] Update Stats to get latest, then unbind from that event and increment. Draw achievement if complete.
  (if (`KismetStringLibrary.IsEmpty` (`self.Achievement Name`))
    (`self.K2_DestroyActor`)
    (else
      (bind (_minprogress _maxprogress) (`UserStats.GetAchievementProgressLimits` (subsystem `UserStats`) (`self.Achievement Name`)))
      (if (>= (`self.Stat`) _maxprogress)
        (`/Game/_Guards/OnlineSubsystem/Achievements/BP_Achievement_Component.Write Achievement` (`self.GetComponentByClass` (`GameplayStatics.GetPlayerController` 0) "/Game/_Guards/OnlineSubsystem/Achievements/BP_Achievement_Component.BP_Achievement_Component_C") (`KismetStringLibrary.Conv_StringToName` (`self.Achievement Name`)))
        ;;[1 1 1] Remove after complete
        (`self.K2_DestroyActor` :!label _label)
        (elif (or (<= _maxprogress 10) (== (mod _stat 10) 0) (`KismetArrayLibrary.Array_Contains` (`self.Always Show Progress`) (`self.Achievement Name`)) (== (`self.Stat`) 1))
          (`UserStats.IndicateAchievementProgress` (`self.Achievement Name`) _stat _maxprogress)
          (goto _label))))))

(fn `Try Store Stats`
  (if (`KismetArrayLibrary.Array_Contains` (`self.Store`) (`self.Stat Name`))
    (`UserStats.StoreStats`)))

(fn `UserConstructionScript`)