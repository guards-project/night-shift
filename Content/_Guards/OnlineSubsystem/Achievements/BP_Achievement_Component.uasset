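; Player controller component that tracks Steam achievements and stats, handling increments, direct writes and owner-client requests from the server.
; Spawns short-lived progressor actors to apply progress, chaining gold-spent and frying-pan tiers, with stat-only progressors once top tiers are earned.
; Gold spent comes from save-game coin deltas, zeroed when a progressor completes to avoid double counting.
; Stores stats on spending and EndPlay, resetting them on version mismatch or debug flag.
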(event `self.ReceiveBeginPlay`
  ;[0.2655 1 0.1643] Reset Debug
  (`self.Bind to Coins Updated`)
  (`self.Check Stat Version`)
  (if (and (not (`KismetSystemLibrary.IsPackagedForDistribution`)) (`self.Reset Steam Progress`))
    (`AchievementQueryCallbackProxy.CacheAchievements` (`GameplayStatics.GetPlayerController` 0)
      (:`OnSuccess`
        _)
      (:`OnFailure`
        _))
    (`UserStats.ResetAllStats` (subsystem `UserStats`) true)))

(event `self.ReceiveEndPlay`
  (params (EndPlayReason :type "EEndPlayReason Enum" :default "Destroyed"))
  ;[0.8148 0.02122 0.02122] When player controller parent is destroye (end of round pre-transition)
  (`UserStats.StoreStats`))

(event `Increment User Stat`
  (params (`Stat Name` :type String) (`Achievement Name` :type String) (`Increment Amount` :type Integer))
  ;[0.07292 0.4411 1] Increment Progress or Grant Achievement
  (`|SpawnActorFromClass` "/Game/_Guards/OnlineSubsystem/Achievements/BP_AchievementProgressor.BP_AchievementProgressor_C" (`KismetMathLibrary.Conv_VectorToTransform` (0.0 0.0 0.0)) "AlwaysSpawn" "MultiplyWithRoot" null `Stat Name` `Achievement Name` `Increment Amount` null))

(event `Write Achievement`
  (params (AchievementName :type Name))
  (bind _returnvalue (`GameplayStatics.GetPlayerController` 0))
  ;[0.07292 0.4411 1] Increment Progress or Grant Achievement
  (`AchievementQueryCallbackProxy.CacheAchievements` _returnvalue
    (:`OnSuccess`
      (`AchievementWriteCallbackProxy.WriteAchievementProgress` _returnvalue AchievementName))))

(event `Spend Progress`
  ;[1 1 1] Coins Spent Binding
  (bind _bachieved (`UserStats.GetAchievement` "Spend_1000"))
  (if _bachieved
    (`self.Spend 2500 Progress`)
    (else
      (bind _returnvalue (`|SpawnActorFromClass` "/Game/_Guards/OnlineSubsystem/Achievements/BP_AchievementProgressor.BP_AchievementProgressor_C" (`KismetMathLibrary.Conv_VectorToTransform` (0.0 0.0 0.0)) "AlwaysSpawn" "MultiplyWithRoot" null "Player_GoldSpent" "Spend_1000" (`self.Last Delta`) null))
      (add `Actor.OnDestroyed` _returnvalue (`|CreateDelegate` :!event `ProgressorComplete`)))))

(event `FryingPanJustice`
  ;[1 1 1] Frying Pan
  (bind _bachieved (`UserStats.GetAchievement` "FryingPan"))
  (if _bachieved
    (`self.FryingPanMaster`)
    (else
      (`|SpawnActorFromClass` "/Game/_Guards/OnlineSubsystem/Achievements/BP_AchievementProgressor.BP_AchievementProgressor_C" (`KismetMathLibrary.Conv_VectorToTransform` (0.0 0.0 0.0)) "AlwaysSpawn" "MultiplyWithRoot" null "Player_FryingPanHits" "FryingPan" 1 null))))

(event `Bind to Coins Updated`
  ;[1 1 1] Coins Spent Binding
  (if (`/Game/_Guards/OnlineSubsystem/BPFL_OnlineSubsystem.Guards Has Online Subsystem`)
    (bind _player_save (`/Game/Blueprints/Core/BPFL_Guards.Get Player Save`))
    (`/Engine/EditorBlueprintResources/StandardMacros.IsValid` _player_save
      (:`Is Valid`
        (add `/Game/Blueprints/Core/PlayerSave/SaveGame_Player.Coins Updated` _player_save (delegate `Coins Updated_Event`))
        (set `self.Last Coins` (`/Game/Blueprints/Core/PlayerSave/SaveGame_Player.Coins` _player_save)))
      (:`Is Not Valid`
        (`KismetSystemLibrary.Delay` 0.2)
        (`self.Bind to Coins Updated`)))))

(event `Coins Updated_Event`
  (params (`Player Save` :type "/Game/Blueprints/Core/PlayerSave/SaveGame_Player Object Reference"))
  (bind _coins (`/Game/Blueprints/Core/PlayerSave/SaveGame_Player.Coins` `Player Save`))
  ;[1 1 1] Coins Spent Binding
  (`|ExecutionSequence`
    (:`then_0`
      (set `self.Last Delta` (- (`self.Last Coins`) _coins))
      (if (> (`self.Last Delta`) 0)
        (`|ExecutionSequence`
          (:`then_0`
            (`self.Spend Progress`))
          (:`then_1`
            (bind _returnvalue (`UserStats.StoreStats` :!label _label))
            (if (not _returnvalue)
              (`KismetSystemLibrary.Delay` 10.0)
              (goto _label))))))
    (:`then_1`
      (set `self.Last Coins` _coins))))

(event `FryingPanMaster`
  ;[1 1 1] Frying Pan
  (bind _bachieved (`UserStats.GetAchievement` "FryingPanMaster"))
  (if _bachieved
    (`|SpawnActorFromClass` "/Game/Blueprints/Core/Components/BP_StatProgressor.BP_StatProgressor_C" (`KismetMathLibrary.Conv_VectorToTransform` (0.0 0.0 0.0)) "Undefined" "MultiplyWithRoot" null "Player_FryingPanHits" 1 null)
    (else
      (`|SpawnActorFromClass` "/Game/_Guards/OnlineSubsystem/Achievements/BP_AchievementProgressor.BP_AchievementProgressor_C" (`KismetMathLibrary.Conv_VectorToTransform` (0.0 0.0 0.0)) "AlwaysSpawn" "MultiplyWithRoot" null "Player_FryingPanHits" "FryingPanMaster" 1 null))))

(event `Spend 2500 Progress`
  ;[1 1 1] Coins Spent Binding
  (bind _bachieved (`UserStats.GetAchievement` "Spend_2500"))
  (if _bachieved
    (`self.Spend 5000 Progress`)
    (else
      (bind _returnvalue (`|SpawnActorFromClass` "/Game/_Guards/OnlineSubsystem/Achievements/BP_AchievementProgressor.BP_AchievementProgressor_C" (`KismetMathLibrary.Conv_VectorToTransform` (0.0 0.0 0.0)) "AlwaysSpawn" "MultiplyWithRoot" null "Player_GoldSpent" "Spend_2500" (`self.Last Delta`) null))
      (add `Actor.OnDestroyed` _returnvalue (`|CreateDelegate` :!event `ProgressorComplete`)))))

(event `ProgressorComplete`
  (params (DestroyedActor :type "Actor Object Reference"))
  ;[1 1 1] Coins Spent Binding
  ;;[1 1 1] If the achievement is newly earned, show the progress bar of the next achievement
  (set `self.Last Delta` 0) ; set last delta to 0 after having applied the delta to progress\notherwise we apply it multiple times to steam
  (bind _asbp_achievement_progressor (cast `/Game/_Guards/OnlineSubsystem/Achievements/BP_AchievementProgressor` DestroyedActor))
  (bind _achievement_name (`/Game/_Guards/OnlineSubsystem/Achievements/BP_AchievementProgressor.Achievement Name` _asbp_achievement_progressor))
  (bind _bachieved (`UserStats.GetAchievement` _achievement_name))
  (if _bachieved
    (switch `string` _achievement_name ; go to next
      (:`Spend_1000`
        (`self.Spend 2500 Progress`))
      (:`Spend_2500`
        (`self.Spend 5000 Progress`)))))

(event `Spend 5000 Progress`
  ;[1 1 1] Coins Spent Binding
  (bind _bachieved (`UserStats.GetAchievement` "Spend_5000"))
  (if _bachieved
    (`|SpawnActorFromClass` "/Game/Blueprints/Core/Components/BP_StatProgressor.BP_StatProgressor_C" (`KismetMathLibrary.Conv_VectorToTransform` (0.0 0.0 0.0)) "Undefined" "MultiplyWithRoot" null "Player_GoldSpent" (`self.Last Delta`) null)
    (else
      (bind _returnvalue (`|SpawnActorFromClass` "/Game/_Guards/OnlineSubsystem/Achievements/BP_AchievementProgressor.BP_AchievementProgressor_C" (`KismetMathLibrary.Conv_VectorToTransform` (0.0 0.0 0.0)) "AlwaysSpawn" "MultiplyWithRoot" null "Player_GoldSpent" "Spend_5000" (`self.Last Delta`) null))
      (add `Actor.OnDestroyed` _returnvalue (`|CreateDelegate` :!event `ProgressorComplete`)))))

(event `Owner Achievement Progress`
  (params (`Stat Name` :type String) (`Achievement Name` :type String) (`Increment Amount` :type Integer :default 1))
  ;[1 1 1] Server RPC owning client progress
  (`|SpawnActorFromClass` "/Game/_Guards/OnlineSubsystem/Achievements/BP_AchievementProgressor.BP_AchievementProgressor_C" (`KismetMathLibrary.Conv_VectorToTransform` (0.0 0.0 0.0)) "AlwaysSpawn" "MultiplyWithRoot" null `Stat Name` `Achievement Name` `Increment Amount` null))

(event `Owner Write Achievement`
  (params (Achievement :type String))
  ;[1 1 1] Server RPC owning client progress
  (`self.Write Achievement` (`KismetStringLibrary.Conv_StringToName` Achievement)))

(event `Check Stat Version`
  ;[1 1 1] Reset Stats
  (if (`/Game/_Guards/OnlineSubsystem/BPFL_OnlineSubsystem.Guards Has Online Subsystem`)
    (`/Game/_Guards/OnlineSubsystem/BPFL_OnlineSubsystem.Request Stats` (delegate `Stats Received`))
    (else
      (`KismetSystemLibrary.K2_SetTimerDelegate` (delegate `Check Stat Version`) 1.0))))

(event `Stats Received`
  (params (Data :type "UserStatsReceived Structure (by ref)"))
  (bind _statversion (`/Game/Blueprints/Core/BP_GameInstance_Template.StatVersion` (cast `/Game/Blueprints/Core/BP_GameInstance_Template` (`GameplayStatics.GetGameInstance`) :!pure true)))
  ;[1 1 1] Reset Stats
  (bind _data (`UserStats.GetStatInt` "Stat_Version"))
  (if (!= _data (`KismetStringLibrary.Conv_StringToInt` _statversion))
    (bind _returnvalue (`UserStats.ResetAllStats` (subsystem `UserStats`) false))
    (if _returnvalue
      (`UserStats.SetStatInt` "Stat_Version" (`KismetStringLibrary.Conv_StringToInt` _statversion))
      (`UserStats.StoreStats`))))