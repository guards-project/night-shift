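; Music component that plays each level's track, looked up by level name in DT_Music with a Default fallback, shortly after begin play.
; The game instance stores the audio component and last track, so repeat requests for the same music are skipped.
; New tracks load asynchronously, then any playing music fades out before a timer swaps the cue's wave parameter and fades the next in.
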(event `self.ReceiveBeginPlay`
  (`KismetSystemLibrary.Delay` 1.0) ; Wait for CVARs
  (bind _menu_music (`self.Get Music For Level`))
  (`self.Play Music` 2.0 _menu_music (`KismetMathLibrary.SelectFloat` 1.0 2.0 (`/Game/Blueprints/Core/BPFL_Guards.Is HUB`))))

(event `Play Next`
  (`AudioComponent.SetWaveParameter` (`self.Get Music Ref`) "Music" (`self.Next Sound`))
  (`AudioComponent.FadeIn` (`self.Music Ref`) (`self.Next Fade In`) 1.0 0.0 "Linear"))

(event `Play Music`
  (params (FadeOutDuration :type "Float (single-precision)" :default 2.0) (Music :type "SoundWave Soft Object Reference") (FadeInDuration :type "Float (single-precision)" :default 2.0))
  (set `self.Next Fade In` FadeInDuration)
  (if (!= Music (`self.Get Last Wav`))
    (`self.Set Last Wav` Music)
    (bind _object (`|LoadAsset` Music)
      (:`Completed`
        (bind _assound_wave (cast `SoundWave` _object))
        (set `self.Next Sound` _assound_wave)
        (if (`AudioComponent.IsPlaying` (`self.Get Music Ref`))
          (`AudioComponent.FadeOut` (`self.Get Music Ref`) FadeOutDuration 0.0 "Linear")
          (`KismetSystemLibrary.K2_SetTimerDelegate` (delegate `Play Next`) FadeOutDuration)
          (else
            (`self.Play Next`)))))))

(event `Stop Music`
  (params (FadeOutDuration :type "Float (single-precision)" :default 2.0))
  (bind _music_ref (`self.Music Ref`)
    (:`then`
      (`AudioComponent.FadeOut` _music_ref FadeOutDuration 0.0 "Linear"))
    (:`else`)))

(fn `Get Last Wav`
  (returns (`Last Music Wav` :type "SoundWave Soft Object Reference"))
  (bind _asbp_game_instance_template (cast `/Game/Blueprints/Core/BP_GameInstance_Template` (`GameplayStatics.GetGameInstance`)))
  (return (`/Game/Blueprints/Core/BP_GameInstance_Template.Last Music Wav` _asbp_game_instance_template)))

(fn `Get Music For Level`
  (returns (`Menu Music` :type "SoundWave Soft Object Reference"))
  ;[1 1 1] Music
  (bind _returnvalue (`GameplayStatics.GetCurrentLevelName` true))
  (bind _returnvalue_2 (`|GetDataTableRow` "/Game/_Guards/Audio/Music/DT_Music.DT_Music" (`KismetStringLibrary.Conv_StringToName` _returnvalue))
    (:`then`
      (return (`.Music_7_6F2518414F46CF96545685A2E6A0057C` (break `/Game/_Guards/Audio/Music/F_LevelMusic` _returnvalue_2))))
    (:`RowNotFound`
      (bind _returnvalue_3 (`|GetDataTableRow` "/Game/_Guards/Audio/Music/DT_Music.DT_Music" "Default")
        (:`then`
          (return (`.Music_7_6F2518414F46CF96545685A2E6A0057C` (break `/Game/_Guards/Audio/Music/F_LevelMusic` _returnvalue_3))))))))

(fn `Get Music Ref`
  (returns (`Music Ref` :type "AudioComponent Object Reference"))
  (bind _music_ref (`self.Music Ref`)
    (:`then`
      (return _music_ref))
    (:`else`
      (bind _asbp_game_instance_template (cast `/Game/Blueprints/Core/BP_GameInstance_Template` (`GameplayStatics.GetGameInstance`)))
      (bind _music (`/Game/Blueprints/Core/BP_GameInstance_Template.Music` _asbp_game_instance_template)
        (:`then`
          (set `self.Music Ref` _music))
        (:`else`
          (bind _returnvalue (`GameplayStatics.CreateSound2D` "/Game/_Guards/Audio/Music/A_Music_Cue.A_Music_Cue" 1.0 1.0 0.0 null true))
          (bind _output_get (set `/Game/Blueprints/Core/BP_GameInstance_Template.Music` _returnvalue _asbp_game_instance_template))
          (set `self.Music Ref` _output_get)))
      (return (`self.Music Ref`)))))

(fn `Set Last Wav`
  (params (`Last Music Wav` :type "SoundWave Soft Object Reference"))
  (bind _asbp_game_instance_template (cast `/Game/Blueprints/Core/BP_GameInstance_Template` (`GameplayStatics.GetGameInstance`)))
  (set `/Game/Blueprints/Core/BP_GameInstance_Template.Last Music Wav` `Last Music Wav` _asbp_game_instance_template))