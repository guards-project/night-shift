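; Voice component for guard AI that plays voice-set lines by row name or ID, attached to itself.
; On authority it randomizes pitch, lowering it for two Undead configs; setting a voice set primes its Death sound.
; Cosmetic-gated playback async-loads DataTable sounds, skips repeats still playing and lets high-priority lines cut off the previous sound.
; Each loaded line also creates noise from its row data, even when playback is skipped.
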(event `self.ReceiveBeginPlay`
  (`/Engine/EditorBlueprintResources/ActorComponentMacros.Switch Has Authority`
    (:`Authority`
      (set `self.Pitch` (`KismetMathLibrary.RandomFloatInRange` 0.8 1.2))
      (bind _asbp_polygon_ai (cast `/Game/Blueprints/Core/PolygonAI/BP_Polygon_AI` (`self.GetOwner`)))
      (add `/Game/Blueprints/Core/BP_Character_Template.Config Updated` _asbp_polygon_ai (delegate `Config Updated_Event`))
      (`self.Config Updated_Event`))))

(event `Config Updated_Event`
  (bind _asbp_polygon_ai (cast `/Game/Blueprints/Core/PolygonAI/BP_Polygon_AI` (`self.GetOwner`)))
  (bind (_datatable _rowname) (break `DataTableRowHandle` (`/Game/Blueprints/Core/BP_Character_Template.Config` _asbp_polygon_ai)))
  (if (or (== _rowname "Undead_Scyther") (== _rowname "Undead_Kingpin"))
    (set `self.Pitch` 0.7)))

(event `Server Set Voice Set`
  (params (`Voice Set` :type "DataTable Object Reference"))
  (bind _output_get (set `self.Voice Set` `Voice Set`))
  (bind _returnvalue (`|GetDataTableRow` _output_get "Death")
    (:`then`
      (bind _object (`|LoadAsset` (`.Sound_10_165D9CBC495FA8B8E8954FB8CAA3DBD8` (break `/Game/_Guards/Audio/VoiceSet/F_Voice` _returnvalue)))
        (:`then`
          (bind _assound_base (cast `SoundBase` _object))
          (`GameplayStatics.PrimeSound` _assound_base))))))

(event `MC Voice`
  (params (RowName :type Name))
  (`self.Play Voice` RowName))

(event `Play Voice by ID`
  (params (ID :type Integer))
  (bind _outrownames (`DataTableFunctionLibrary.GetDataTableRowNames` (`self.Voice Set`)))
  (if (`KismetArrayLibrary.Array_IsValidIndex` _outrownames ID)
    (`self.Play Voice` (`|GetArrayItem` _outrownames ID))
    (else
      (`KismetSystemLibrary.PrintString` "Requested Voice ID is Invalid"))))

(event `Play Voice`
  (params (RowName :type Name))
  (`/Engine/EditorBlueprintResources/StandardMacros.Can Execute Cosmetic Events`
    (:`True`
      (bind _returnvalue (`|GetDataTableRow` (`self.Voice Set`) RowName)
        (:`then`
          (bind (_sound _noisedata) (break `/Game/_Guards/Audio/VoiceSet/F_Voice` _returnvalue))
          (bind _object (`|LoadAsset` _sound)
            (:`Completed`
              (bind _assound_base (cast `SoundBase` _object))
              (`|ExecutionSequence`
                (:`then_0`
                  (if (`self.Can Play` RowName)
                    (`self.Play Sound` _assound_base (`self.Should Stop Previous Sound` RowName))
                    (set `self.Last Sound Name` RowName)))
                (:`then_1`
                  (`/Game/Blueprints/Core/PolygonAI/SenseData/BPFL_Noise.Create Noise` (`self.GetOwner`) (`self.K2_GetComponentLocation`) _noisedata))))))))))

(fn `Can Play`
  (params (`New Sound` :type Name))
  (returns (Allow :type Boolean))
  (bind _last_sound (`self.Last Sound`)
    (:`then`
      (if (`AudioComponent.IsPlaying` _last_sound)
        (return (!= (`local.New Sound`) (`self.Last Sound Name`)))
        (else
          (return true))))
    (:`else`
      (return true))))

(fn `Play Sound`
  (params (`Sound Base` :type "SoundBase Object Reference") (`Should Cancel last` :type Boolean))
  (`|ExecutionSequence`
    (:`then_0`
      (if `Should Cancel last`
        (bind _last_sound (`self.Last Sound`)
          (:`then`
            (`AudioComponent.Stop` _last_sound))
          (:`else`))))
    (:`then_1`
      (bind _sound_base (`local.Sound Base`)
        (:`then`
          (bind _returnvalue (`GameplayStatics.SpawnSoundAttached` _sound_base self "None" (0.0 0.0 0.0) (struct) "SnapToTarget" false 1.0 (`self.Pitch`) 0.0 null null))
          (bind _output_get (set `self.Last Sound` _returnvalue))
          (`/Engine/EditorBlueprintResources/StandardMacros.IsValid` _output_get
            (:`Is Valid`
              (`AudioComponent.Play` _output_get 0.0))))
        (:`else`)))))

(fn `Should Stop Previous Sound`
  (params (`New Sound` :type Name))
  (returns (OutputPin :type Boolean))
  (return (`KismetArrayLibrary.Array_Contains` (`self.High Prio Sounds`) `New Sound`)))