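; Player controller for replay viewing that creates and shows the replay screen widget for the local player.
; On BeginPlay it adds the widget at high Z-order, enables the mouse cursor and sets Game and UI input.
; Each tick it applies the inverse of the replay subsystem's playback speed as time dilation to itself and the spectator pawn, offsetting playback speed, and makes both tickable while paused.
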(event `self.ReceiveBeginPlay`
  (if (`self.IsLocalController`)
    (`self.Create Replay Screen`)))

(event `self.ReceiveTick`
  (params (DeltaSeconds :type "Float (single-precision)"))
  (bind _returnvalue (`self.GetSpectatorPawn`))
  (bind _returnvalue_2 (/ 1.0 (`KismetMathLibrary.FMax` (`GuardsReplaySubsystem.GetPlaybackSpeed` (subsystem `GuardsReplaySubsystem`)) 0.0001)))
  ;[1 1 1] Dilate PC
  (set `self.CustomTimeDilation` _returnvalue_2)
  (`self.SetTickableWhenPaused` true)
  ;[1 1 1] Dilate Spectator
  (`/Engine/EditorBlueprintResources/StandardMacros.IsValid` _returnvalue
    (:`Is Valid`
      (set `Actor.CustomTimeDilation` _returnvalue_2 _returnvalue)
      (`self.SetTickableWhenPaused` _returnvalue true))))

(event `Create Replay Screen`
  (bind _returnvalue (`GameplayStatics.GetPlayerController` 0))
  (if (`self.IsLocalPlayerController` _returnvalue)
    (bind _returnvalue_2 (`|CreateWidget` "/Game/_Guards/UserInterface/Replays/W_ReplayScreen.W_ReplayScreen_C" _returnvalue))
    (set `self.Replay Screen` _returnvalue_2)
    (bind _replay_screen (`self.Replay Screen`)
      (:`then`
        (`UserWidget.AddToViewport` _replay_screen 5000)
        (`WidgetBlueprintLibrary.SetInputMode_GameAndUIEx` self _replay_screen "LockAlways" false)
        (set `self.bShowMouseCursor` true)
        (`Widget.SetVisibility` (`self.Replay Screen`) "Visible"))
      (:`else`))))

(fn `UserConstructionScript`)