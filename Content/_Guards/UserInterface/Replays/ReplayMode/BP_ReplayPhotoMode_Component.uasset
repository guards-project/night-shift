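; Replay photo mode component that lets players adjust a camera and capture high-resolution screenshots.
; Entering creates the photo mode widget, passing itself in, and creates an auto-playing spectator sequence; exiting removes the widget and blends back to the spectator pawn.
; Setters forward lens, color, effect and LUT grading values to PhotoPawn, while roll rotates the camera directly.
; TakeShot runs HighResShot with a clamped multiplier between pre- and post-capture controller notifications.
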(fn `CameraRoll`
  (params (Value :type "Float (double-precision)"))
  (bind _camroll (`self.CamRoll`))
  (bind (_relativerotation_roll _relativerotation_pitch _relativerotation_yaw) (`KismetMathLibrary.BreakRotator` (`SceneComponent.RelativeRotation` (`self.Camera`))))
  (`SceneComponent.K2_SetRelativeRotation` (`self.Camera`) (`KismetMathLibrary.MakeRotator` (`KismetMathLibrary.Lerp` (- _camroll (* _camroll 2.0)) _camroll (`local.Value`)) _relativerotation_pitch _relativerotation_yaw) false false)
  (return))

(fn `EnterPhotoMode`
  (params (Camera :type "CineCameraComponent Object Reference"))
  (set `self.Camera` Camera)
  (bind _returnvalue (`|CreateWidget` "/Game/_Guards/UserInterface/Replays/ReplayMode/W_ReplayPhotomode.W_ReplayPhotomode_C" null self))
  (bind _output_get (set `self.Photo Mode Widget` _returnvalue))
  (`UserWidget.AddToViewport` _output_get 5000)
  (`LevelSequencePlayer.CreateLevelSequencePlayer` "/Game/_Guards/UserInterface/Replays/ReplayMode/LS_Spectator.LS_Spectator" (make `MovieSceneSequencePlaybackSettings` true)))

(fn `ExitPhotoMode`
  (bind _returnvalue (`GameplayStatics.GetPlayerController` 0))
  (`Widget.RemoveFromParent` (`self.Photo Mode Widget`))
  (`PlayerController.SetViewTargetWithBlend` _returnvalue (`PlayerController.GetSpectatorPawn` _returnvalue) 0.2 "VTBlend_Linear" 0.0 true))

(fn `GetPauseRule`
  (returns (bCanPause :type Boolean))
  (return (`KismetSystemLibrary.IsStandalone`)))

(fn `GetPlayerCount`
  (returns (`Num Humans` :type Integer))
  (locals (LocalCount :type Integer))
  ;[1 1 1] Get all players in player array, if no bot then add to count
  (for _array_element (`GameStateBase.PlayerArray` (`GameplayStatics.GetGameState`))
    (`/Engine/EditorBlueprintResources/StandardMacros.IsValid` _array_element
      (:`Is Valid`
        (if (not (`PlayerState.bIsABot` _array_element))
          (set `local.LocalCount` (+ (`local.LocalCount`) 1))))))
  (return (`local.LocalCount`)))

(fn `IsInPhotomode`
  (returns (bCondition :type Boolean))
  ;[1 1 1] return is in photomode
  (return (`self.bIsInPhotoMode`)))

(fn `Set Aperture`
  (params (Alpha :type "Float (double-precision)"))
  ;[1 1 1] Pass aperture
  (`/Game/Photomode/Blueprints/BP_PhotoModePawn.Set Aperture` (`self.PhotoPawn`) Alpha)
  (return))

(fn `SetColorGrading`
  (params (Index :type Integer))
  ;[1 1 1] Pass color grading
  (`/Game/Photomode/Blueprints/BP_PhotoModePawn.SetColorGrading` (`self.PhotoPawn`) (select `/Game/Photomode/Enums/EColorThemes` (cast `/Game/Photomode/Enums/EColorThemes` (`KismetMathLibrary.Conv_IntToByte` Index)) :`NewEnumerator0` "/Game/Photomode/Textures/CrossProcessLUT.CrossProcessLUT" :`NewEnumerator1` "/Game/Photomode/Textures/portaesque.portaesque" :`NewEnumerator2` "/Game/Photomode/Textures/proviaesqueLUT.proviaesqueLUT" :`NewEnumerator3` "/Game/Photomode/Textures/velviaesque.velviaesque" :`NewEnumerator4` "/Game/Photomode/Textures/LUT_Red1.LUT_Red1" :`NewEnumerator5` "/Game/Photomode/Textures/LUT_LightBlue1.LUT_LightBlue1" :`NewEnumerator7` "/Game/Photomode/Textures/LUT_Snowy.LUT_Snowy" :`NewEnumerator8` "/Game/Photomode/Textures/LUT_RainyDay.LUT_RainyDay" :!type "Texture Object Reference"))
  (return))

(fn `SetColorGradingIntensity`
  (params (Alpha :type "Float (double-precision)"))
  ;[1 1 1] Pass color grading intensity
  (`/Game/Photomode/Blueprints/BP_PhotoModePawn.SetColorGradingIntensity` (`self.PhotoPawn`) Alpha)
  (return))

(fn `SetColors`
  (params (Color :type "/Game/Photomode/Enums/EPhotoColors Enum" :default "NewEnumerator0") (Value :type "Float (double-precision)"))
  (bind _photopawn (`self.PhotoPawn`))
  (bind _photopawn_2 (`self.PhotoPawn`))
  (bind _value (`local.Value`))
  ;[1 1 1] Pass colors
  (`self.PhotoPawn`
    (:`then`
      (switch `/Game/Photomode/Enums/EPhotoColors` Color
        (:`NewEnumerator0`
          (`/Game/Photomode/Blueprints/BP_PhotoModePawn.SetSaturation` _photopawn _value)
          (return))
        (:`NewEnumerator1`
          (`/Game/Photomode/Blueprints/BP_PhotoModePawn.SetGamma` _photopawn _value)
          (return))
        (:`NewEnumerator2`
          (`/Game/Photomode/Blueprints/BP_PhotoModePawn.SetGain` _photopawn_2 _value)
          (return))
        (:`NewEnumerator3`
          (`/Game/Photomode/Blueprints/BP_PhotoModePawn.SetContrast` _photopawn_2 _value)
          (return))))
    (:`else`)))

(fn `SetEffect`
  (params (Effect :type "/Game/Photomode/Enums/EPhotoEffects Enum" :default "NewEnumerator0") (Value :type "Float (double-precision)"))
  (locals (LocalValue :type "Float (double-precision)"))
  (bind _photopawn (`self.PhotoPawn`))
  (bind _photopawn_2 (`self.PhotoPawn`))
  (bind _photopawn_3 (`self.PhotoPawn`))
  (bind _localvalue (`local.LocalValue`))
  (bind _value (`local.Value`))
  ;[1 1 1] Set effect
  (`self.PhotoPawn`
    (:`then`
      (switch `/Game/Photomode/Enums/EPhotoEffects` (`local.Effect`)
        (:`NewEnumerator0`
          (`/Game/Photomode/Blueprints/BP_PhotoModePawn.SetVignette` _photopawn _value)
          (return))
        (:`NewEnumerator1`
          (`/Game/Photomode/Blueprints/BP_PhotoModePawn.SetBloom` _photopawn _value)
          (return))
        (:`NewEnumerator2`
          (`/Game/Photomode/Blueprints/BP_PhotoModePawn.SetLensFlare` _photopawn_2 _value)
          (return))
        (:`NewEnumerator3`
          (`/Game/Photomode/Blueprints/BP_PhotoModePawn.SetLensFlareBokeh` _photopawn_2 _value)
          (return))
        (:`NewEnumerator4`
          (`/Game/Photomode/Blueprints/BP_PhotoModePawn.SetGrain` _photopawn_3 _localvalue)
          (return))
        (:`NewEnumerator5`
          (`/Game/Photomode/Blueprints/BP_PhotoModePawn.SetFringe` _photopawn_3 _localvalue)
          (return))))
    (:`else`)))

(fn `SetFocalDistance`
  (params (Alpha :type "Float (double-precision)"))
  ;[1 1 1] Pass focal distance
  (`/Game/Photomode/Blueprints/BP_PhotoModePawn.SetFocalDistance` (`self.PhotoPawn`) Alpha)
  (return))

(fn `SetFocalLength`
  (params (Alpha :type "Float (double-precision)"))
  ;[1 1 1] Pass focal length
  (`/Game/Photomode/Blueprints/BP_PhotoModePawn.SetFocalLength` (`self.PhotoPawn`) Alpha)
  (return))

(fn `TakeShot`
  (params (MagnifierValue :type "Float (double-precision)"))
  ;[1 1 1] Take screenshot with multiplier
  (message `/Game/Photomode/Blueprints/BPI_PhotoModeInterface.Pre Photo Taken` (`self.PlayerController`))
  (`KismetSystemLibrary.ExecuteConsoleCommand` (`KismetStringLibrary.Concat_StrStr` "HighResShot " (`KismetStringLibrary.Conv_IntToString` (`KismetMathLibrary.Clamp` (`KismetMathLibrary.FCeil` MagnifierValue) 1 4))) (`self.PlayerController`))
  (message `/Game/Photomode/Blueprints/BPI_PhotoModeInterface.Post Photo Taken` (`self.PlayerController`))
  (return))