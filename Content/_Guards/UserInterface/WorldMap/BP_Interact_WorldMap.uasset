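; Interactable world map actor that opens a level select menu for the local player who uses it.
; Interacting pushes the UI widget onto the menu stack, using a CanDraw flag reset on widget deactivation to block duplicates.
; It also turns the player's view toward the map in third person with preset zoom, offset and FOV.
; Interaction is refused while the widget is in the viewport; an older host-only restriction is disconnected.
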(event `/Game/Primer/Primer_Interaction/BPI_Interact.Execute Interact`
  (params (User :type "Controller Object Reference"))
  (`self.Open Level Select` User))

(event `Draw UI`
  (params (Player :type "PlayerController Object Reference"))
  (if (`self.Can Draw`)
    (set `self.Can Draw` false)
    (bind _ui (`self.UI`)
      (:`then`
        (bind (_commonstack _stack_menu) (`/Game/_Guards/UserInterface/Menus/Stack/BPFL_CommonStack.Push Menu` _ui))
        (`KismetSystemLibrary.Delay` 0.2)
        (bind _returnvalue (`CommonActivatableWidgetContainerBase.GetActiveWidget` _stack_menu))
        (set `self.UI Ref` _returnvalue)
        (add `CommonActivatableWidget.BP_OnWidgetDeactivated` _returnvalue (delegate `BP_OnWidgetDeactivated_Event`)))
      (:`else`))))

(event `BP_OnWidgetDeactivated_Event`
  (set `self.Can Draw` true))

(fn `Get Can Interact`
  (returns (ReturnValue :type Boolean))
  (bind _ui_ref (`self.UI Ref`)
    (:`then`
      (return (not (`Widget.IsInViewport` _ui_ref))))
    (:`else`
      (return true))))

(fn `Get Interact Text`
  (returns (Text :type Text))
  (return (`self.Interact Text`)))

(fn `Open Level Select`
  (params (InputPin :type "Controller Object Reference"))
  (if (`Controller.IsLocalController` InputPin)
    (bind _asplayer_controller (cast `PlayerController` InputPin))
    (`self.Draw UI` _asplayer_controller)
    (`self.Setup Camera` _asplayer_controller)))

(fn `Setup Camera`
  (params (Player :type "Controller Object Reference"))
  ;[1 1 1] Control the camera on the player because we want to make surrrre we're overr shoulder & relative
  (bind _asbp_character_template_player (cast `/Game/Blueprints/Core/BP_Character_Template_Player` (`Controller.K2_GetPawn` Player)))
  (bind (_returnvalue_roll _returnvalue_pitch _returnvalue_yaw) (`KismetMathLibrary.BreakRotator` (`KismetMathLibrary.FindLookAtRotation` (`self.K2_GetActorLocation` _asbp_character_template_player) (`self.K2_GetActorLocation`))))
  (`Controller.SetControlRotation` (`GameplayStatics.GetPlayerController` 0) (`KismetMathLibrary.MakeRotator` _returnvalue_roll (`self.Camera Pitch`) (+ _returnvalue_yaw (`self.Camera Yaw`))))
  (set `/Game/Blueprints/Core/BP_Character_Template_Player.Target Zoom` (`self.Camera Zoom`) _asbp_character_template_player)
  (`/Game/Blueprints/Core/BP_Character_Template_Player.Set Third Person` _asbp_character_template_player true)
  (set `SpringArmComponent.SocketOffset` (`self.Camera Offset`) (`/Game/Blueprints/Core/BP_Character_Template_Player.SpringArm` _asbp_character_template_player))
  (`CameraComponent.SetFieldOfView` (`/Game/Blueprints/Core/BP_Character_Template_Player.Camera` _asbp_character_template_player) (`self.Camera FOV`)))

(fn `UserConstructionScript`
  (`parent.UserConstructionScript`))