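; Component that tracks and persists day-based cooldowns for the world map's Reduce, Reroll and Freeze crisis abilities.
; On BeginPlay the authority loads or creates the save, decrements each cooldown by one (floored at zero) in the HUB, then saves.
; Setting a cooldown reassigns the replicated array to force its OnRep, fires the activation event and saves.
; The OnRep and activation event broadcast dispatchers for listeners.
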(event `self.ReceiveBeginPlay`
  (`/Engine/EditorBlueprintResources/ActorComponentMacros.Switch Has Authority`
    (:`Authority`
      (`self.Init Cooldowns`))))

(event `MC Ability Activated`
  (params (ID :type Integer))
  (`self.Crisis Ability Activated` self ID))

(fn `Get Cooldown For Ability`
  (params (Index :type "Integer (by ref)"))
  (returns (Value :type Integer))
  ;[1 1 1] 0 = Reduce
  ; 1 = Reroll
  ; 2 = Freeze
  (return (`|GetArrayItem` (`self.Ability Cooldown`) Index)))

(fn `Get Crisis Ability Save`
  (returns (ReturnValue :type "/Game/_Guards/UserInterface/WorldMap/Crisis/BP_SaveGame_CrisisAbility Object Reference"))
  (bind _slot (`self.Slot`))
  (bind _returnvalue (`GameplayStatics.DoesSaveGameExist` _slot))
  (if _returnvalue
    (bind _returnvalue_2 (`GameplayStatics.LoadGameFromSlot` _slot))
    (bind _asbp_save_game_crisis_ability (cast `/Game/_Guards/UserInterface/WorldMap/Crisis/BP_SaveGame_CrisisAbility` _returnvalue_2))
    (bind _output_get (set `self.Crisis Ability Save` _asbp_save_game_crisis_ability))
    (return _output_get)
    (else
      (`GameplayStatics.DeleteGameInSlot` (`self.Slot`))
      (bind _returnvalue_3 (`GameplayStatics.CreateSaveGameObject` "/Game/_Guards/UserInterface/WorldMap/Crisis/BP_SaveGame_CrisisAbility.BP_SaveGame_CrisisAbility_C"))
      (bind _output_get_2 (set `self.Crisis Ability Save` _returnvalue_3))
      (return _output_get_2))))

(fn `Init Cooldowns`
  (locals (`L Save` :type "/Game/_Guards/UserInterface/WorldMap/Crisis/BP_SaveGame_CrisisAbility Object Reference") (`L Cooldowns` :type "Array of Integer"))
  (bind _l_save (`local.L Save`))
  (bind _returnvalue (`self.Get Crisis Ability Save`))
  (set `local.L Save` _returnvalue)
  (set `local.L Cooldowns` (`/Game/_Guards/UserInterface/WorldMap/Crisis/BP_SaveGame_CrisisAbility.Ability | Cooldown` _returnvalue))
  (if (`/Game/Blueprints/Core/BPFL_Guards.Is HUB`)
    (for (_array_element _array_index) (`local.L Cooldowns`)
      (`KismetArrayLibrary.Array_Set` (`local.L Cooldowns`) _array_index (`KismetMathLibrary.Max` (- _array_element 1)))))
  (set `/Game/_Guards/UserInterface/WorldMap/Crisis/BP_SaveGame_CrisisAbility.Ability | Cooldown` (`local.L Cooldowns`) _l_save)
  (`self.Save` _l_save)
  (set `self.Ability Cooldown` (`local.L Cooldowns`)))

(fn `OnRep_Ability Cooldown`
  (`self.Crisis Abilities Updated` self))

(fn `Save`
  (params (SaveGameObject :type "SaveGame Object Reference"))
  (`GameplayStatics.SaveGameToSlot` SaveGameObject (`self.Slot`)))

(fn `Set Cooldown For Ability`
  (params (Index :type Integer) (Days :type "Integer (by ref)"))
  (locals (`L Save` :type "/Game/_Guards/UserInterface/WorldMap/Crisis/BP_SaveGame_CrisisAbility Object Reference") (`L Cooldowns` :type "Array of Integer"))
  ;[1 1 1] 0 = Reduce
  ; 1 = Reroll
  ; 2 = Freeze
  (`KismetArrayLibrary.Array_Set` (`self.Ability Cooldown`) Index Days) ; doesn't trigger onrep
  (set `self.Ability Cooldown` (`self.Ability Cooldown`)) ; so force trigger onrep
  (`self.MC Ability Activated` (`local.Index`))
  (bind _returnvalue (`self.Get Crisis Ability Save`))
  (bind _output_get (set `local.L Save` _returnvalue))
  (set `/Game/_Guards/UserInterface/WorldMap/Crisis/BP_SaveGame_CrisisAbility.Ability | Cooldown` (`self.Ability Cooldown`) (`local.L Save`))
  (`self.Save` _output_get))