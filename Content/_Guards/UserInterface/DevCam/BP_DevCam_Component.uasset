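; Controller component that provides a developer free camera for slow-motion views and high-resolution screenshots, captured with H.
; EnterDevCam halts the character, spawns or reuses a BP_DevCam above the pawn's eye point, possesses it and nearly freezes time with slomo, offset by a huge CustomTimeDilation on the camera.
; ExitDevCam repossesses the saved pawn and restores normal speed.
; The FlipFlop toggle and screenshot-folder launch are unwired.
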(event `Key|H`
  (params (Key :type "Key Structure"))
  (:`Pressed`
    (`KismetSystemLibrary.ExecuteConsoleCommand` "HighResShot 2" (`GameplayStatics.GetPlayerController` 0))
    (`Screenshots.TriggerScreenshot`)))

(event `Key|P`
  (params (Key :type "Key Structure"))
  ;[1 1 1] Input from player
)

(event `Enter DevCam`
  (bind _devcam (`self.DevCam`))
  (bind (_outlocation _outrotation) (`Actor.GetActorEyesViewPoint` (`Controller.K2_GetPawn` (cast `Controller` (`self.GetOwner`) :!pure true))))
  ;[1 1 1] Enter exit devcam on server
  (bind _ascontroller (cast `Controller` (`self.GetOwner`)))
  (bind _returnvalue (`Controller.K2_GetPawn` _ascontroller))
  (`/Engine/EditorBlueprintResources/StandardMacros.IsValid` _returnvalue
    (:`Is Valid`
      (bind _output_get (set `self.Last Pawn` _returnvalue))
      (bind _ascharacter (cast `Character` _output_get))
      (`MovementComponent.StopMovementImmediately` (`Character.CharacterMovement` _ascharacter)))
    (:`Is Not Valid`
      _))
  (`self.DevCam`
    (:`then`
      _)
    (:`else`
      (bind _returnvalue_2 (`|SpawnActorFromClass` "/Game/_Guards/UserInterface/DevCam/BP_DevCam.BP_DevCam_C" (`KismetMathLibrary.MakeTransform` (0.0 0.0 0.0)) "AlwaysSpawn" "MultiplyWithRoot" null null))
      (set `self.DevCam` _returnvalue_2)))
  (`Actor.K2_SetActorLocationAndRotation` (`self.DevCam`) (+ _outlocation (0.0 0.0 50.0)) _outrotation false false)
  (`Controller.Possess` (cast `Controller` (`self.GetOwner`) :!pure true) _devcam)
  (set `Actor.CustomTimeDilation` 10000.0 _devcam)
  (`KismetSystemLibrary.ExecuteConsoleCommand` "DisableAllScreenMessages" (`GameplayStatics.GetPlayerController` 0))
  (`KismetSystemLibrary.ExecuteConsoleCommand` "slomo .0001" (`GameplayStatics.GetPlayerController` 0)))

(event `Exit DevCam`
  ;[1 1 1] Enter exit devcam on server
  (`MovementComponent.StopMovementImmediately` (`/Game/_Guards/UserInterface/DevCam/BP_DevCam.FloatingPawnMovement` (`self.DevCam`)))
  (bind _last_pawn (`self.Last Pawn`)
    (:`then`
      (`Controller.Possess` (cast `Controller` (`self.GetOwner`) :!pure true) _last_pawn)
      (`KismetSystemLibrary.ExecuteConsoleCommand` "slomo 1" (`GameplayStatics.GetPlayerController` 0))
      (set `Actor.CustomTimeDilation` 1.0 _last_pawn))
    (:`else`)))