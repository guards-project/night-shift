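; BP_DevCam is a free-flying developer camera pawn that hides the player HUD while a local player controls it.
; On controller change it collapses the first W_PlayerHUD found, restoring it when the local controller leaves.
; Enhanced Input actions drive planar movement along actor axes, world-vertical height and look with inverted pitch input.
; The mouse wheel raises or lowers the FloatingPawnMovement max speed within a clamped range.
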(event `self.ReceiveControllerChanged`
  (params (OldController :type "Controller Object Reference") (NewController :type "Controller Object Reference"))
  (`/Engine/EditorBlueprintResources/StandardMacros.IsValid` NewController
    (:`Is Valid`
      (if (`Controller.IsLocalPlayerController` NewController)
        (bind _foundwidgets (`WidgetBlueprintLibrary.GetAllWidgetsOfClass` "/Game/_Guards/UserInterface/GameHUD/W_PlayerHUD.W_PlayerHUD_C"))
        (if (`KismetArrayLibrary.Array_IsValidIndex` _foundwidgets)
          (`Widget.SetVisibility` (`|GetArrayItem` _foundwidgets) "Collapsed"))))
    (:`Is Not Valid`
      (`/Engine/EditorBlueprintResources/StandardMacros.IsValid` OldController
        (:`Is Valid`
          (if (`Controller.IsLocalPlayerController` OldController)
            (bind _foundwidgets_2 (`WidgetBlueprintLibrary.GetAllWidgetsOfClass` "/Game/_Guards/UserInterface/GameHUD/W_PlayerHUD.W_PlayerHUD_C"))
            (if (`KismetArrayLibrary.Array_IsValidIndex` _foundwidgets_2)
              (`Widget.SetVisibility` (`|GetArrayItem` _foundwidgets_2) "HitTestInvisible"))))))))

(event `EnhancedInput|/Game/Blueprints/Input/IA_Move`
  (params (ActionValue :type "Vector2D Structure") (ElapsedSeconds :type "Float (double-precision)") (TriggeredSeconds :type "Float (double-precision)") (InputAction :type "InputAction Object Reference" :default "/Game/Blueprints/Input/IA_Move.IA_Move"))
  (bind (_x _y) (`KismetMathLibrary.BreakVector2D` ActionValue))
  (:`Triggered`
    (`self.AddMovementInput` (`self.GetActorRightVector`) _x)
    (`self.AddMovementInput` (`self.GetActorForwardVector`) _y)))

(event `EnhancedInput|/Game/Blueprints/Input/IA_Look`
  (params (ActionValue :type "Vector2D Structure") (ElapsedSeconds :type "Float (double-precision)") (TriggeredSeconds :type "Float (double-precision)") (InputAction :type "InputAction Object Reference" :default "/Game/Blueprints/Input/IA_Look.IA_Look"))
  (bind (_x _y) (`KismetMathLibrary.BreakVector2D` ActionValue))
  (:`Triggered`
    (`self.AddControllerYawInput` _x)
    (`self.AddControllerPitchInput` (* _y -1.0))))

(event `EnhancedInput|/Game/Blueprints/Input/IA_Height`
  (params (ActionValue :type "Float (double-precision)") (ElapsedSeconds :type "Float (double-precision)") (TriggeredSeconds :type "Float (double-precision)") (InputAction :type "InputAction Object Reference" :default "/Game/Blueprints/Input/IA_Height.IA_Height"))
  (:`Triggered`
    (`self.AddMovementInput` (0.0 0.0 1.0) ActionValue)))

(event `InputAxisKey|MouseWheelAxis`
  (params (AxisValue :type "Float (single-precision)"))
  (bind _floatingpawnmovement (`self.FloatingPawnMovement`))
  (set `FloatingPawnMovement.MaxSpeed` (`KismetMathLibrary.FClamp` (+ (`MovementComponent.GetMaxSpeed` _floatingpawnmovement) (* 30.0 AxisValue)) 0.0 5000.0) _floatingpawnmovement))

(fn `UserConstructionScript`)