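; BP_Interact_WidgetPopup is an interactable that opens a popup widget when a user interacts with it.
; ExecuteInteract runs only for a local controller and pushes WidgetClass onto a menu stack, guarded by CanDraw against duplicate popups.
; After a short delay it caches the stack's active widget and binds its deactivation event, which re-enables CanDraw.
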(event `/Game/Primer/Primer_Interaction/BPI_Interact.Execute Interact`
  (params (User :type "Controller Object Reference"))
  (if (`Controller.IsLocalController` User)
    (if (`self.Can Draw`)
      (set `self.Can Draw` false)
      (bind (_commonstack _stack_menu) (`/Game/_Guards/UserInterface/Menus/Stack/BPFL_CommonStack.Push Menu` (`self.Widget Class`)))
      (`KismetSystemLibrary.Delay` 0.2)
      (bind _returnvalue (`CommonActivatableWidgetContainerBase.GetActiveWidget` _stack_menu))
      (set `self.UI Ref` _returnvalue)
      (add `CommonActivatableWidget.BP_OnWidgetDeactivated` _returnvalue (delegate `BP_OnWidgetDeactivated_Event`)))))

(event `BP_OnWidgetDeactivated_Event`
  (set `self.Can Draw` true))

(fn `UserConstructionScript`
  (`parent.UserConstructionScript`))