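; Tutorial controls Blueprint that shows either gamepad or PC control widgets to match the player's current input method.
; On BeginPlay it binds to the CommonInputSubsystem's input method change event and applies the current input type immediately, retrying after a short delay until the player controller and subsystem are valid.
; Each change toggles visibility between WidgetGamepad and WidgetPC, with every non-gamepad input showing the PC version.
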(event `self.ReceiveBeginPlay`
  (`self.Bind to Input Changed`))

(event `Bind to Input Changed`
  (bind _returnvalue (`GameplayStatics.GetPlayerController` 0))
  (bind _returnvalue_2 (pcsubsystem `CommonInputSubsystem` _returnvalue))
  (`/Engine/EditorBlueprintResources/StandardMacros.IsValid` _returnvalue
    (:`Is Valid`
      (`/Engine/EditorBlueprintResources/StandardMacros.IsValid` _returnvalue_2
        (:`Is Valid`
          (add `CommonInputSubsystem.OnInputMethodChanged` _returnvalue_2 (delegate `OnInputMethodChanged_Event`))
          (`self.OnInputMethodChanged_Event` (`CommonInputSubsystem.GetCurrentInputType` _returnvalue_2)))
        (:`Is Not Valid`
          (`KismetSystemLibrary.Delay` 0.2 :!label _label)
          (`self.Bind to Input Changed`))))
    (:`Is Not Valid`
      (goto _label))))

(event `OnInputMethodChanged_Event`
  (params (bNewInputType :type "ECommonInputType Enum" :default "MouseAndKeyboard"))
  (bind _returnvalue (`|EnumEquality` bNewInputType "Gamepad"))
  (`SceneComponent.SetVisibility` (`self.WidgetGamepad`) _returnvalue false)
  (`SceneComponent.SetVisibility` (`self.WidgetPC`) (not _returnvalue) false))

(fn `UserConstructionScript`)