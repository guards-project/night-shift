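; BP_Cage is a cage actor in the goblin camp map with a breakable door and a collision blocker for AI visibility.
; On BeginPlay, only on the authority, it casts the CageDoor child actor to BP_FractureActor and binds to its fractured event.
; When the door fractures, it disables collision on VisibilityBlockerForAI, so the blocker no longer obstructs AI.
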(event `self.ReceiveBeginPlay`
  (`parent.ReceiveBeginPlay`)
  (`/Engine/EditorBlueprintResources/ActorMacros.Switch Has Authority`
    (:`Authority`
      (bind _asbp_fracture_actor (cast `/Game/Blueprints/Fracture/FractureCore/BP_FractureActor` (`ChildActorComponent.ChildActor` (`self.CageDoor`))))
      (add `/Game/Blueprints/Fracture/FractureCore/BP_FractureActor.Fractured` _asbp_fracture_actor (delegate `Fractured_Event`)))))

(event `Fractured_Event`
  (params (Actor :type "/Game/Blueprints/Fracture/FractureCore/BP_FractureActor Object Reference"))
  (`PrimitiveComponent.SetCollisionEnabled` (`self.VisibilityBlockerForAI`) "NoCollision"))

(fn `UserConstructionScript`
  (`parent.UserConstructionScript`))