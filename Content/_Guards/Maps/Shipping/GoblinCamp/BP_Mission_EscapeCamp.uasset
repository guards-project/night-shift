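; Mission actor for the goblin camp escape that resets each player's pawn on possession.
; On the server at BeginPlay, it binds to the game mode's player-join callback and replays it for players already present.
; Each controller's possessed-pawn change clears that player character's default inventory items and sets its health to 1.0.
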(event `self.ReceiveBeginPlay`
  (`parent.ReceiveBeginPlay`)
  (`/Engine/EditorBlueprintResources/ActorMacros.Switch Has Authority`
    (:`Authority`
      (bind _asbp_game_mode_template (cast `/Game/Blueprints/Core/BP_GameMode_Template` (`GameplayStatics.GetGameMode`)))
      (add `/Game/Blueprints/Core/Components/BP_PlayerJoinLeaveCallback.Player Joined` (`/Game/Blueprints/Core/BP_GameMode_Template.BP_PlayerJoinLeaveCallback` _asbp_game_mode_template) (delegate `Player Joined_Event`))
      (for _array_element (`GameStateBase.PlayerArray` (`GameplayStatics.GetGameState`))
        (bind _returnvalue (`self.GetOwner` _array_element))
        (`/Engine/EditorBlueprintResources/StandardMacros.IsValid` _returnvalue
          (:`Is Valid`
            (bind _ascontroller (cast `Controller` _returnvalue))
            (`self.Player Joined_Event` _ascontroller)))))))

(event `Player Joined_Event`
  (params (Controller :type "Controller Object Reference") (PlayerState :type "PlayerState Object Reference"))
  (bind _returnvalue (`Controller.K2_GetPawn` Controller))
  (add `Controller.OnPossessedPawnChanged` Controller (delegate `OnPossessedPawnChanged_Event`))
  (`/Engine/EditorBlueprintResources/StandardMacros.IsValid` _returnvalue
    (:`Is Valid`
      (`self.OnPossessedPawnChanged_Event` null _returnvalue))))

(event `OnPossessedPawnChanged_Event`
  (params (OldPawn :type "Pawn Object Reference") (NewPawn :type "Pawn Object Reference"))
  (bind _asbp_character_template_player (cast `/Game/Blueprints/Core/BP_Character_Template_Player` NewPawn))
  (`KismetArrayLibrary.Array_Clear` (`/Game/Blueprints/Items/BP_Inventory_Component.Default Items` (`/Game/Blueprints/Core/BP_Character_Template.BP_Inventory_Component` _asbp_character_template_player)))
  (`/Game/Blueprints/Core/Components/BP_Health_Component.Set Health` (`/Game/Blueprints/Core/BP_Character_Template.BP_Health_Component` _asbp_character_template_player) 1.0))

(fn `UserConstructionScript`
  (`parent.UserConstructionScript`))